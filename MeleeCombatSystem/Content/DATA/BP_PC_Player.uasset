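; Player character Blueprint that hides parts of its body mesh when visible leg or chest equipment is worn.
; PlayerIconUpdate calls the parent, then LegsEquiped and ChestEquiped scan the EquipmentComponet Equiped map for matching slot types, ignoring items flagged EquipmentInvisible.
; Each check swaps its mesh material slots to transparent variants, or restores chain mail and old-man materials when nothing qualifies.
; The construction script attaches PlayerIcon to the mesh's spine_03 socket.
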(event EventBeginPlay
  (|CallParentFunction))

(event Collision|EventActorBeginOverlap
  (params (OtherActor :type Actor%20Object%20Reference)))

(event EventTick
  (params (DeltaSeconds :type Float%20%28single-precision%29))
  (|CallParentFunction DeltaSeconds) ; This node is disabled and will not be called.\nDrag off pins to build functionality.
)

(event EventPlayerIconUpdate
  (|CallParentFunction)
  (CallFunction|LegsEquiped?)
  (CallFunction|ChestEquiped?))

(fn ConstructionScript
  (|CallParentFunction)
  (Transformation|AttachComponentToComponent (Variables|Default|GetPlayerIcon) (Variables|Character|GetMesh) "spine_03" "KeepRelative" "KeepRelative" "KeepRelative" true))

(fn LegsEquiped?
  (bind _equipmentcomponet (Variables|Default|GetEquipmentComponet))
  (bind _equiped (Variables|/Game/DATA/Blueprints/Components/EquipmentComponet.EquipmentComponet_C|GetEquiped _equipmentcomponet))
  (Variables|Default|SetLegsEquiped false)
  (bind _keys (Utilities|Map|Keys _equiped))
  (for _array_element _keys
    (Utilities|IsValid (.equipeditem (.Value (Utilities|Map|Find _equiped _array_element)))
      (:Is%20Valid
        (if (or (Utilities|Enum|Equal(Enum) (.equiptype (.Value (Utilities|Map|Find _equiped _array_element))) "NewEnumerator5") (Utilities|Enum|Equal(Enum) "NewEnumerator6" (.equiptype (.Value (Utilities|Map|Find _equiped _array_element)))))
          (if (not (Variables|/Game/DATA/Blueprints/Actors/BP_BaseEquippable.BP_BaseEquippable_C|GetEquipmentInvisible (.equipeditem (.Value (Utilities|Map|Find _equiped _array_element)))))
            (Variables|Default|SetLegsEquiped true)
            (Rendering|Material|SetMaterial (Variables|Character|GetMesh) 3 "/Game/DATA/Materials/MasterMaterials/MM_MainDerivatives/MI_ChainMailTrans.MI_ChainMailTrans")
            (Rendering|Material|SetMaterial (Variables|Character|GetMesh) 5 "/Game/DATA/Materials/MasterMaterials/MM_MainDerivatives/MI_Transparent.MI_Transparent"))))))
  (if (not (Variables|Default|GetLegsEquiped))
    (Rendering|Material|SetMaterial (Variables|Character|GetMesh) 3 "/Game/DATA/Materials/MasterMaterials/MM_MainDerivatives/MI_ChainMail.MI_ChainMail")
    (Rendering|Material|SetMaterial (Variables|Character|GetMesh) 5 "/Game/DATA/Materials/MasterMaterials/MM_MainDerivatives/MI_oldMan.MI_oldMan")))

(fn ChestEquiped?
  (bind _equipmentcomponet (Variables|Default|GetEquipmentComponet))
  (bind _equiped (Variables|/Game/DATA/Blueprints/Components/EquipmentComponet.EquipmentComponet_C|GetEquiped _equipmentcomponet))
  (Variables|Default|SetChestEquiped false)
  (bind _keys (Utilities|Map|Keys _equiped))
  (for _array_element _keys
    (Utilities|IsValid (.equipeditem (.Value (Utilities|Map|Find _equiped _array_element)))
      (:Is%20Valid
        (if (Utilities|Enum|Equal(Enum) (.equiptype (.Value (Utilities|Map|Find _equiped _array_element))) "NewEnumerator1")
          (if (not (Variables|/Game/DATA/Blueprints/Actors/BP_BaseEquippable.BP_BaseEquippable_C|GetEquipmentInvisible (.equipeditem (.Value (Utilities|Map|Find _equiped _array_element)))))
            (Variables|Default|SetChestEquiped true)
            (Rendering|Material|SetMaterial (Variables|Character|GetMesh) 4 "/Game/DATA/Materials/MasterMaterials/MM_MainDerivatives/MI_Transparent.MI_Transparent"))))))
  (if (not (Variables|Default|GetChestEquiped))
    (Rendering|Material|SetMaterial (Variables|Character|GetMesh) 4 "/Game/DATA/Materials/MasterMaterials/MM_MainDerivatives/MI_oldMan.MI_oldMan")))