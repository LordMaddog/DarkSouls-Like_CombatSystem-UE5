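; Frost giant boss Blueprint that adds death, reset and long-range attack behavior on top of its parent class.
; Death plays a troll death montage, and both death and reset remove the boss health UI.
; Long-range attacks spawn an aimed charged smash ability actor at the boss and send it a dash attack message, throttled by a DoOnce that resets after a short delay.
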(event EventBeginPlay
  (|CallParentFunction) ; This node is disabled and will not be called.\nDrag off pins to build functionality.
)

(event Collision|EventActorBeginOverlap
  (params (OtherActor :type Actor%20Object%20Reference))
  (|CallParentFunction OtherActor) ; This node is disabled and will not be called.\nDrag off pins to build functionality.
)

(event EventTick
  (params (DeltaSeconds :type Float%20%28single-precision%29))
  (|CallParentFunction DeltaSeconds) ; This node is disabled and will not be called.\nDrag off pins to build functionality.
)

(event EventDie
  (|CallParentFunction)
  (Animation|PlayAnimMontage "/Game/DATA/AI/FrostGiantBoss/Animations/ExoGame_Troll_Death__Montage.ExoGame_Troll_Death__Montage" 1.0 "None")
  (bind _bosshealthui (Variables|Default|GetBossHealthUI)
    (:then
      (Widget|RemovefromParent _bosshealthui))
    (:else)))

(event EventLongRangeAttacks
  (bind _self self)
  (Utilities|FlowControl|DoOnce false :!label _label
    (:Completed
      (bind _returnvalue (Game|SpawnActorfromClass "/Game/DATA/Blueprints/Abilities/GA_GiantAimChargedSmash.GA_GiantAimChargedSmash_C" (Transformation|GetActorTransform) "Undefined" "MultiplyWithRoot" _self 0 _self))
      (Class|GamePlayAbilitiesBPI|DashAttack(Message) _returnvalue 1e+03)
      (Utilities|FlowControl|Delay 2.0)
      (goto _label Reset))))

(event EventReset
  (|CallParentFunction)
  (bind _bosshealthui (Variables|Default|GetBossHealthUI)
    (:then
      (Widget|RemovefromParent _bosshealthui))
    (:else)))

(fn ConstructionScript
  (|CallParentFunction))