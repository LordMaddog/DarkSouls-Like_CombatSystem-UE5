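; AI controller for BP_MasterAI pawns that runs the pawn's behavior tree and manages enemy targeting.
; On possess it binds the combat component's toggle to the bCombatEnabled blackboard key.
; Perception updates check the first two stimuli, target sensed actors lacking matching gameplay tags, and notify the pawn.
; If no target qualifies, it waits SearchDuration, then clears TargetedEnemy unless still visible by sight.
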(event OnPerceptionUpdated(AIPerception)
  (params (UpdatedActors :type Array%20of%20Actor%20Object%20References))
  (bind _successfully_sensed (CallFunction|UpdatePerception UpdatedActors))
  (if (not _successfully_sensed)
    (Utilities|FlowControl|Delay (Variables|Default|GetSearchDuration))
    (if (not (CallFunction|CanStillSee?))
      (CallFunction|SetTargetActor))))

(event Custom|OncombatToggled
  (params (CombatEnabled :type Boolean))
  (AI|Components|Blackboard|SetValueasBool (Variables|Default|GetBlackboard) (Utilities|Name|MakeLiteralName "bCombatEnabled") CombatEnabled))

(event EventBeginPlay)

(event EventTick
  (params (DeltaSeconds :type Float%20%28single-precision%29)))

(event EventPossess
  (params (PossessedPawn :type Pawn%20Object%20Reference))
  (bind _asbp_master_ai (Utilities|Casting|CastToBP_MasterAI PossessedPawn))
  (Variables|Default|SetMaster%20AI _asbp_master_ai)
  (EventDispatchers|BindEventtoOnCombatToggled (Variables|/Game/DATA/BP_PC.BP_PC_C|GetCombatComponent (Variables|Default|GetMaster%20AI)) (EventDispatchers|CreateEvent :!event Custom|OncombatToggled))
  (AI|RunBehaviorTree (Variables|/Game/DATA/AI/BP_MasterAI.BP_MasterAI_C|GetBehabiorTree (Variables|Default|GetMaster%20AI))))

(fn ConstructionScript)

(fn UpdatePerception
  (params (PerceivedActors :type Array%20of%20Actor%20Object%20References))
  (for _array_element PerceivedActors
    (LocalVariables|SetL_sensedActor _array_element)
    (bind _info (Class|AIPerceptionComponent|GetActorsPerception (Variables|Default|GetAIPerception) (LocalVariables|GetL_sensedActor)))
    (for (_array_element_2 _array_index) (.LastSensedStimuli (Utilities|Struct|BreakActorPerceptionBlueprintInfo _info))
      (LocalVariables|SetL_AIStimilus _array_element_2)
      (switch int _array_index
        (:0
          (if (.bSuccessfullySensed (Utilities|Struct|BreakAIStimulus (LocalVariables|GetL_AIStimilus)))
            (bind _returnvalue (Class|GameplayTagBPI|HasMatchingGamplayTag(Message) (LocalVariables|GetL_sensedActor) (Variables|/Game/DATA/BP_PC.BP_PC_C|GetOwnedGamePlayTags (Variables|Default|GetMaster%20AI))))
            (if (not _returnvalue)
              (CallFunction|SetTargetActor (LocalVariables|GetL_sensedActor))
              (return true))))
        (:1
          (if (.bSuccessfullySensed (Utilities|Struct|BreakAIStimulus (LocalVariables|GetL_AIStimilus)))
            (bind _returnvalue_2 (Class|GameplayTagBPI|HasMatchingGamplayTag(Message) (LocalVariables|GetL_sensedActor) (Variables|/Game/DATA/BP_PC.BP_PC_C|GetOwnedGamePlayTags (Variables|Default|GetMaster%20AI))))
            (if (not _returnvalue_2)
              (CallFunction|SetTargetActor (LocalVariables|GetL_sensedActor))
              (return true))))))
    (return false)))

(fn SetTargetActor
  (params (NewTargetActor :type Actor%20Object%20Reference))
  (AI|Components|Blackboard|SetValueasObject (Variables|Default|GetBlackboard) (Utilities|Name|MakeLiteralName "TargetedEnemy") NewTargetActor)
  (bind _master_ai (Variables|Default|GetMaster%20AI)
    (:then
      (Default|OnTargetSet _master_ai NewTargetActor))
    (:else)))

(fn CanStillSee?
  (for _array_element (Class|AIPerceptionComponent|GetCurrentlyPerceivedActors (Variables|Default|GetAIPerception) "/Script/AIModule.AISense_Sight")
    (if (== _array_element (AI|Components|Blackboard|GetValueasObject (Variables|Default|GetBlackboard) (Utilities|Name|MakeLiteralName "TargetedEnemy")))
      (LocalVariables|SetL_Seen true)))
  (if (LocalVariables|GetL_Seen)
    (return true)
    (else
      (return false))))