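; Base AI combat character for NPCs, registered on the map as an enemy, that drives patrol and death state through its Blackboard.
; Range, block, ability and enchant events feed the combat component, while action gameplay tags select montages by index or at random.
; Damage from instigators without matching tags is reported to AI damage sensing.
; A fallback hand weapon, partly marked deprecated, handles socket swaps, hit damage and physics on death.
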(event OnHit(CollosionComponent)
  (params (HitResult :type Hit%20Result%20Structure))
  (bind _hitactor (Collision|BreakHitResult HitResult))
  ;[1 1 1] InCharacterWeaponDamage(depricated)
  (Variables|Default|SetHitResult HitResult)
  (bind _returnvalue (Class|CombatBPI|CanReciveDamage(Message) _hitactor))
  (if _returnvalue
    (Game|Damage|ApplyPointDamage _hitactor (Default|GetSubStats (Variables|Default|GetStatsComponent) "NewEnumerator11") (Transformation|GetActorForwardVector) (Variables|Default|GetHitResult) (Pawn|GetController) self (Variables|Default|GetDamage%20Type%20Class))))

(event OnCombatToggled(CombatComponent)
  (params (CombatEnabled :type Boolean))
  ;[1 1 1] InCharacterWeapon(depricated)
  (if (CallFunction|UseHandWeapon?)
    (Transformation|AttachComponentToComponent (Variables|Default|GetWeapon) (Variables|Character|GetMesh) (select CombatEnabled (Variables|Default|GetHandSocketName) (Variables|Default|GetAttachSocket%20Name)) "SnapToTarget" "SnapToTarget" "SnapToTarget" true)))

(event Custom|OnTargetSet
  (params (SensedActor :type Actor%20Object%20Reference))
  ;[1 1 1] SetAITarget
  (Default|SetTargetActor (Variables|Default|GetTargetingComponent) SensedActor))

(event Custom|Simulate%20%20Physics
  ;[1 1 1] InCharacterWeapon(depricated)
  (if (CallFunction|UseHandWeapon?)
    (Collision|SetCollisionProfileName (Variables|Default|GetWeapon) "PhysicsActor" true :!class /Script/Engine.PrimitiveComponent)
    (Physics|SetSimulatePhysics (Variables|Default|GetWeapon) true)))

(event Custom|GAAction
  (params (GAAbility :type GA%20Base%20Ability%20Class%20Reference))
  ;[1 1 1] NPC Combat Attacks
  (Default|UseGA (Variables|Default|GetCombatComponent) GAAbility))

(event Custom|CloseRangeAttacks
  ;[1 1 1] NPC Combat Attacks
)

(event Custom|MediumRangeAttacks
  ;[1 1 1] NPC Combat Attacks
)

(event Custom|FarRangeAttacks
  ;[1 1 1] NPC Combat Attacks
)

(event Custom|LongRangeAttacks
  ;[1 1 1] NPC Combat Attacks
  (CallFunction|RotatetoTarget)
  (Utilities|FlowControl|Delay 0.2)
  (Default|DashAttack (Variables|Default|GetCombatComponent)))

(event Custom|Block
  ;[1 1 1] NPC Combat Attacks
  (Default|Block (Variables|Default|GetCombatComponent))
  (Variables|Default|SetBlockPressed true))

(event Custom|BlockStop
  ;[1 1 1] NPC Combat Attacks
  (Variables|Default|SetBlockPressed false)
  (Default|SetBlockingState (Variables|Default|GetCombatComponent) false))

(event Custom|EnchantWeapon
  (params (Activate :type Boolean) (MagicType :type E_MagicType%20Enum :default "NewEnumerator0"))
  ;[1 1 1] NPC Combat Attacks
  (Default|Enchant (Variables|Default|GetCombatComponent) Activate MagicType))

(event Custom|Patrol
  (params (ShouldPatrol :type Boolean) (PatrolType :type Integer))
  (bind _self self)
  (bind _returnvalue (AI|GetAIController _self))
  (bind _returnvalue_2 (AI|GetBlackboard _returnvalue))
  ;[1 1 1] Patrol
  (AI|Components|Blackboard|SetValueasBool _returnvalue_2 (Utilities|Name|MakeLiteralName "Patrol") ShouldPatrol)
  (Class|BlackboardComponent|SetValueasInt _returnvalue_2 (Utilities|Name|MakeLiteralName "PatrolType") PatrolType))

(event EventBeginPlay
  (bind _mapcomponent (Variables|Default|GetMapComponent))
  ;[1 1 1] Event BeginPlay
  (|CallParentFunction)
  (Variables|/Game/DATA/Blueprints/Components/CollosionComponent.CollosionComponent_C|SetGamplayTagsToIgnore (Variables|Default|GetCollosionComponent) (Variables|Default|GetOwnedGamePlayTags))
  (if (CallFunction|UseHandWeapon?)
    (Default|SetCollisionMesh (Variables|Default|GetCollosionComponent) (Variables|Default|GetWeapon)))
  (Utilities|FlowControl|Delay 1.0)
  (Default|SetIconName _mapcomponent (Variables|/Game/DATA/Blueprints/Components/StatsComponent.StatsComponent_C|GetNpc%20Name (Variables|Default|GetStatsComponent)))
  (Default|InitDataIcon _mapcomponent "Enemy"))

(event EventTick
  (params (DeltaSeconds :type Float%20%28single-precision%29))
  ;[1 1 1] Event Tick
  (|CallParentFunction DeltaSeconds) ; This node is disabled and will not be called.\nDrag off pins to build functionality.
)

(event EventActivateCollision
  (params (CollisionPart :type E_CollisionPart%20Enum :default "NewEnumerator0") (LeftHand :type Boolean))
  ;[1 1 1] InCharacterWeapon(depricated)
  (|CallParentFunction CollisionPart LeftHand)
  (if (CallFunction|UseHandWeapon?)
    (Default|EnableCollision (Variables|Default|GetCollosionComponent))))

(event Game|Damage|EventPointDamage
  (params (Damage :type Float%20%28single-precision%29) (DamageType :type Damage%20Type%20Object%20Reference) (HitLocation :type Vector :default "0, 0, 0") (HitNormal :type Vector :default "0, 0, 0") (HitComponent :type Primitive%20Component%20Object%20Reference) (BoneName :type Name :default "None") (ShotFromDirection :type Vector :default "0, 0, 0") (InstigatedBy :type Controller%20Object%20Reference) (DamageCauser :type Actor%20Object%20Reference) (HitInfo :type Hit%20Result%20Structure%20%28by%20ref%29))
  (bind _returnvalue (Pawn|GetControlledPawn InstigatedBy))
  ;[1 1 1] Recive Damage
  (|CallParentFunction Damage DamageType HitLocation HitNormal HitComponent BoneName ShotFromDirection InstigatedBy DamageCauser HitInfo)
  (Utilities|IsValid InstigatedBy
    (:Is%20Valid
      (bind _gameplaytags (Class|GameplayTagBPI|GetOwnedGamplayTags(Message) InstigatedBy))
      (if (not (GameplayTags|HasAnyTags _gameplaytags (Variables|Default|GetOwnedGamePlayTags) true))
        (Utilities|IsValid _returnvalue
          (:Is%20Valid
            (Class|AISenseDamage|ReportDamageEvent self _returnvalue Damage HitLocation HitLocation "None")))))))

(event EventDeactivateCollision
  (params (CollisionPart :type E_CollisionPart%20Enum :default "NewEnumerator0"))
  ;[1 1 1] InCharacterWeapon(depricated)
  (|CallParentFunction CollisionPart)
  (if (CallFunction|UseHandWeapon?)
    (Default|DisableCollision (Variables|Default|GetCollosionComponent))))

(event EventDie
  ;[1 1 1] InCharacterWeapon(depricated)
  (|CallParentFunction)
  (CallFunction|SetDead true)
  (if (CallFunction|UseHandWeapon?)
    (CallFunction|SimulatePhysics)))

(fn ConstructionScript
  (|CallParentFunction)
  (Variables|Default|SetPreview%20Mesh (Variables|/Script/Engine.SkeletalMeshComponent|GetSkeletalMeshAsset (Variables|Character|GetMesh))))

(fn GetActionMontage
  (params (ActionTag :type Gameplay%20Tag%20Structure))
  (|SwitchGameplayTag ActionTag
    (:Character.Action.Attack.Light%20Attack
      (return (Variables|Montages|GetLightAttackMontages)))
    (:Character.Action.Attack.ChargeAttack
      (return (Variables|Montages|GetMediumRangeAttackMontages)))
    (:Character.Action.Attack.Heavy%20Attack
      (return (Variables|Montages|GetHeavyAttackMontages)))
    (:Character.Action.Dodge
      (return (Variables|Montages|GetDodgeMontages)))
    (:Character.Action.EnterCombat
      (return (Utilities|Array|MakeArray (Variables|Montages|GetEnterCombat))))
    (:Character.Action.ExitCombat
      (return (Utilities|Array|MakeArray (Variables|Montages|GetExitCombat))))
    (:Character.Action.Attack.Ranged
      (return (Variables|Montages|GetRangeAttackMontages)))))

(fn AIProformAttack
  (params (AttackIndex :type Integer) (bRandomIndex :type Boolean) (AttackType :type Gameplay%20Tag%20Structure))
  (bind _combatcomponent (Variables|Default|GetCombatComponent))
  (LocalVariables|SetL_attackMontages (CallFunction|GetActionMontage AttackType))
  (bind _output_get (LocalVariables|SetL_attackMontage (select bRandomIndex (.OutItem (Utilities|Array|Random (LocalVariables|GetL_attackMontages))) (Utilities|Array|Get(acopy) (LocalVariables|GetL_attackMontages) (select (> AttackIndex (Utilities|Array|LastIndex (LocalVariables|GetL_attackMontages))) 0 AttackIndex)))))
  (Utilities|IsValid _output_get
    (:Is%20Valid
      (Default|SetState _combatcomponent AttackType)
      (Default|SetCurrentAction _combatcomponent AttackType)
      (Animation|PlayAnimMontage (LocalVariables|GetL_attackMontage) 1.0 "None")
      (bind _result (Math|Integer|IncrementInt (Variables|Initialization|GetAttackCount))
        (:%20%20
          (if (> _result (Utilities|Array|LastIndex (LocalVariables|GetL_attackMontages)))
            (Variables|Initialization|SetAttackCount 0)))))
    (:Is%20Not%20Valid
      (Development|PrintString (Utilities|String|Append "Index: " (Utilities|String|ToString(Integer) AttackIndex) " Is Not Valid")))))

(fn AIProformAction
  (params (CharacterActions :type Gameplay%20Tag%20Structure) (CharacterState :type Gameplay%20Tag%20Structure) (MontageIndex :type Integer) (RandomIndex :type Boolean))
  (bind _combatcomponent (Variables|Default|GetCombatComponent))
  (LocalVariables|SetL_ActionMontages (CallFunction|GetActionMontage CharacterActions))
  (Utilities|IsValid (select RandomIndex (.OutItem (Utilities|Array|Random (LocalVariables|GetL_ActionMontages))) (Utilities|Array|Get(acopy) (LocalVariables|GetL_ActionMontages) (select (> MontageIndex (Utilities|Array|LastIndex (LocalVariables|GetL_ActionMontages))) 0 MontageIndex)))
    (:Is%20Valid
      (LocalVariables|SetL_ActionMontage 0)
      (Default|SetState _combatcomponent CharacterState)
      (Default|SetCurrentAction _combatcomponent CharacterActions)
      (Animation|PlayAnimMontage (LocalVariables|GetL_ActionMontage) 1.0 "None"))
    (:Is%20Not%20Valid
      (Development|PrintString (Utilities|String|Append "Index: " (Utilities|String|ToString(Integer) MontageIndex) " Is Not Valid")))))

(fn PreformCombatAttack
  (params (AttackType :type Gameplay%20Tag%20Structure) (SetState :type Gameplay%20Tag%20Structure) (AttackIndex :type Integer) (bRandomIndex :type Boolean))
  (bind _combatcomponent (Variables|Default|GetCombatComponent))
  (LocalVariables|SetL_attackMontages (CallFunction|GetActionMontage AttackType))
  (bind _output_get (LocalVariables|SetL_attackMontage (select bRandomIndex (.OutItem (Utilities|Array|Random (LocalVariables|GetL_attackMontages))) (Utilities|Array|Get(acopy) (LocalVariables|GetL_attackMontages) (select (> AttackIndex (Utilities|Array|LastIndex (LocalVariables|GetL_attackMontages))) 0 AttackIndex)))))
  (Utilities|IsValid _output_get
    (:Is%20Valid
      (Default|SetState _combatcomponent SetState)
      (Default|SetCurrentAction _combatcomponent AttackType)
      (bind _returnvalue (Animation|Montage|MontagePlay (Components|SkeletalMesh|GetAnimInstance (Variables|Character|GetMesh)) (LocalVariables|GetL_attackMontage) (Default|GetSubStats (Variables|Default|GetStatsComponent) "NewEnumerator19") "Duration" 0.0 true))
      (LocalVariables|SetL_AttackDuration _returnvalue)
      (bind _result (Math|Integer|IncrementInt (Variables|Initialization|GetAttackCount))
        (:%20%20
          (if (> _result (Utilities|Array|LastIndex (LocalVariables|GetL_attackMontages)))
            (Variables|Initialization|SetAttackCount 0))
          (return (LocalVariables|GetL_AttackDuration)))))
    (:Is%20Not%20Valid
      (Development|PrintString (Utilities|String|Append "Index: " (Utilities|String|ToString(Integer) AttackIndex) " Is Not Valid")))))

(fn NotLivingHit)

(fn PreformCombatAction
  (params (ActionTag :type Gameplay%20Tag%20Structure) (SateTag :type Gameplay%20Tag%20Structure) (MontageIndex :type Integer) (bRandomItemIndex :type Boolean))
  (bind _combatcomponent (Variables|Default|GetCombatComponent))
  (LocalVariables|SetL_attackMontages (CallFunction|GetActionMontage ActionTag))
  (bind _output_get (LocalVariables|SetL_attackMontage (select bRandomItemIndex (.OutItem (Utilities|Array|Random (LocalVariables|GetL_attackMontages))) (Utilities|Array|Get(acopy) (LocalVariables|GetL_attackMontages) (select (> MontageIndex (Utilities|Array|LastIndex (LocalVariables|GetL_attackMontages))) 0 MontageIndex)))))
  (Utilities|IsValid _output_get
    (:Is%20Valid
      (Default|SetState _combatcomponent ActionTag)
      (Default|SetCurrentAction _combatcomponent ActionTag)
      (bind _returnvalue (Animation|Montage|MontagePlay (Components|SkeletalMesh|GetAnimInstance (Variables|Character|GetMesh)) (LocalVariables|GetL_attackMontage) (Default|GetSubStats (Variables|Default|GetStatsComponent) "NewEnumerator19") "Duration" 0.0 true))
      (LocalVariables|SetL_AttackDuration _returnvalue)
      (bind _result (Math|Integer|IncrementInt (Variables|Initialization|GetAttackCount))
        (:%20%20
          (if (> _result (Utilities|Array|LastIndex (LocalVariables|GetL_attackMontages)))
            (Variables|Initialization|SetAttackCount 0))
          (return (LocalVariables|GetL_AttackDuration)))))
    (:Is%20Not%20Valid
      (Development|PrintString (Utilities|String|Append "Index: " (Utilities|String|ToString(Integer) MontageIndex) " Is Not Valid")))))

(fn UseHandWeapon?
  (return (and (Utilities|IsValid (Variables|Default|GetWeapon)) (not (Utilities|IsValid (Default|GetMainWeapon (Variables|Default|GetCombatComponent)))))))

(fn SetDead
  (params (bDead? :type Boolean))
  (if (!= bDead? (Variables|Default|GetbDead))
    (bind _output_get (Variables|Default|SetbDead bDead?))
    (AI|Components|Blackboard|SetValueasBool (AI|GetBlackboard (AI|GetAIController self)) (Utilities|Name|MakeLiteralName "bDead") _output_get)))

(fn GetDead
  (return (Variables|Default|GetbDead)))