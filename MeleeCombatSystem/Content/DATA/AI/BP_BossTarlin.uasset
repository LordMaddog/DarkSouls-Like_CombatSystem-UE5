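; Tarlin boss AI character that adds a boss health bar and a built-in weapon mesh to its parent's behavior.
; The bar joins the player's HUD at BeginPlay and shows while the boss has a valid target and is not dead.
; Without an equipped main weapon, the mesh switches sockets on combat toggle and follows attack collision windows.
; Collision hits apply point damage from the boss's stats.
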(event OnHit(CollosionComponent)
  (params (HitResult :type Hit%20Result%20Structure))
  (bind _hitactor (Collision|BreakHitResult HitResult))
  ;[1 1 1] InCharacterWeaponDamage
  (Variables|Default|SetHitResult HitResult)
  (bind _returnvalue (Class|CombatBPI|CanReciveDamage(Message) _hitactor))
  (if _returnvalue
    (Game|Damage|ApplyPointDamage _hitactor (Default|GetSubStats (Variables|Default|GetStatsComponent) "NewEnumerator11") (Transformation|GetActorForwardVector) (Variables|Default|GetHitResult) (Pawn|GetController) self (Variables|Default|GetDamage%20Type%20Class))))

(event OnCombatToggled(CombatComponent)
  (params (CombatEnabled :type Boolean))
  ;[1 1 1] InCharacterWeapon
  (Utilities|IsMainWeaponNotValidandHandWeaponIsValid
    (:true
      (Transformation|AttachComponentToComponent (Variables|Default|GetWeapon) (Variables|Character|GetMesh) (select CombatEnabled (Variables|Default|GetHandSocketName) (Variables|Default|GetAttachSocket%20Name)) "SnapToTarget" "SnapToTarget" "SnapToTarget" true))))

(event Custom|SetBossHealthVisibility
  (params (Visible? :type Boolean))
  (bind _bosshealthui (Variables|Default|GetBossHealthUI)
    (:then
      (Variables|/Script/UMG.Widget|SetVisibility _bosshealthui (select (and Visible? (Default|GetCurrentStateNotEqualAny (Variables|Default|GetCombatComponent) "(GameplayTags=((TagName=\"Character.State.Dead\")))")) "Visible" "Hidden")))
    (:else)))

(event Custom|SimulatePhysics
  ;[1 1 1] InCharacterWeapon
  (Utilities|IsMainWeaponNotValidandHandWeaponIsValid
    (:true
      (Collision|SetCollisionProfileName (Variables|Default|GetWeapon) "PhysicsActor" true :!class /Script/Engine.PrimitiveComponent)
      (Physics|SetSimulatePhysics (Variables|Default|GetWeapon) true))))

(event EventBeginPlay
  (|CallParentFunction)
  (Default|SetCollisionMesh (Variables|Default|GetCollosionComponent) (Variables|Default|GetWeapon))
  (bind _asbp_pc (Utilities|Casting|CastToBP_PC (Game|GetPlayerCharacter 0)))
  (bind _returnvalue (UserInterface|CreateWidget "/Game/DATA/UI/HUD/WB_BossHealth.WB_BossHealth_C" (Game|GetPlayerController 0) (Variables|Default|GetStatsComponent)))
  (Variables|Default|SetBossHealthUI _returnvalue)
  (Utilities|IsThisValid (Variables|/Game/DATA/BP_PC.BP_PC_C|GetInventory _asbp_pc) 1e+01
    (:Is%20Valid
      (Widget|Panel|AddChild (Variables|/Game/DATA/UI/Inventory/WBP_MainWidget.WBP_MainWidget_C|GetBossHpBarWindow (Variables|/Game/DATA/Blueprints/Actors/Inventory/BP_Inventory.BP_Inventory_C|GetMainWidget (Variables|/Game/DATA/BP_PC.BP_PC_C|GetInventory _asbp_pc))) (Variables|Default|GetBossHealthUI)))))

(event Collision|EventActorBeginOverlap
  (params (OtherActor :type Actor%20Object%20Reference))
  (|CallParentFunction OtherActor))

(event EventTick
  (params (DeltaSeconds :type Float%20%28single-precision%29))
  (|CallParentFunction DeltaSeconds))

(event EventActivateCollision
  (params (CollisionPart :type E_CollisionPart%20Enum :default "NewEnumerator0") (LeftHand :type Boolean))
  ;[1 1 1] InCharacterWeapon
  (|CallParentFunction CollisionPart LeftHand)
  (Utilities|IsMainWeaponNotValidandHandWeaponIsValid
    (:true
      (Default|EnableCollision (Variables|Default|GetCollosionComponent)))))

(event EventDeactivateCollision
  (params (CollisionPart :type E_CollisionPart%20Enum :default "NewEnumerator0"))
  ;[1 1 1] InCharacterWeapon
  (|CallParentFunction CollisionPart)
  (Utilities|IsMainWeaponNotValidandHandWeaponIsValid
    (:true
      (Default|DisableCollision (Variables|Default|GetCollosionComponent)))))

(event EventDie
  ;[1 1 1] InCharacterWeapon
  (|CallParentFunction)
  (Utilities|IsMainWeaponNotValidandHandWeaponIsValid
    (:true
      (CallFunction|SimulatePhysics0))))

(event EventOnTargetSet
  (params (SensedActor :type Actor%20Object%20Reference))
  (|CallParentFunction SensedActor)
  (CallFunction|SetBossHealthVisibility (Utilities|IsValid SensedActor)))

(fn ConstructionScript
  (|CallParentFunction))

(fn SimulatePhysics0)