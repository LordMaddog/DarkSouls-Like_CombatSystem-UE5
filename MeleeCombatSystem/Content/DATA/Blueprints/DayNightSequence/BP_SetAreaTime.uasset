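; Trigger volume that shifts the day sequence's time of day to a set hour when the player enters.
; On box overlap it reads the current time from the Day Sequence actor, then a timeline lerps it to Hours24, replaying on each player entry.
; ToCastOrNotToCast identifies the player through a character-info message and the combat component's IsPlayer flag, caching the reference for later overlaps.
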(event OnComponentBeginOverlap(Box)
  (params (OverlappedComponent :type Primitive%20Component%20Object%20Reference) (OtherActor :type Actor%20Object%20Reference) (OtherComp :type Primitive%20Component%20Object%20Reference) (OtherBodyIndex :type Integer) (bFromSweep :type Boolean) (SweepResult :type Hit%20Result%20Structure%20%28by%20ref%29))
  (bind _returnvalue (WorldSubsystems|GetDaySequenceSubsystem))
  (bind _returnvalue_2 (Class|DaySequenceSubsystem|GetDaySequenceActor _returnvalue true))
  (bind _isplayer (CallFunction|ToCastorNottoCast OtherActor))
  (if _isplayer
    (Variables|Default|SetCurrentTime (Class|DaySequenceActor|GetTimeOfDay _returnvalue_2))
    (bind _lerptonewtime (Timeline|Timeline PlayFromStart)
      (:Update
        (Class|DaySequenceActor|SetTimeOfDay _returnvalue_2 (Math|Float|Lerp (Variables|Default|GetCurrentTime) (Variables|Default|GetHours%2824%29) _lerptonewtime))))))

(fn ConstructionScript)

(fn ToCastorNottoCast
  (params (InActor :type Actor%20Object%20Reference))
  (Utilities|IsValid (Variables|Default|GetPlayer)
    (:Is%20Valid
      (if (== (Variables|Default|GetPlayer) InActor)
        _
        (else
          (return false))))
    (:Is%20Not%20Valid
      (bind _character (Class|CombatBPI|GetCharacterInfo(Message) InActor))
      (Utilities|IsValid _character
        (:Is%20Valid
          (if (Variables|/Game/DATA/Blueprints/Components/CombatComponent.CombatComponent_C|GetIsPlayer (Variables|/Game/DATA/BP_PC.BP_PC_C|GetCombatComponent _character))
            (Variables|Default|SetPlayer _character)
            (else
              (return false))))
        (:Is%20Not%20Valid
          (return false)))))
  (return true))