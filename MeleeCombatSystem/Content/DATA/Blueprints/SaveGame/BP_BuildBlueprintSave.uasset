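; BP_BuildBlueprintSave stores a set of selected builds as a reusable record of a build blueprint, judging by its name and SaveBluePrint function.
; SaveBluePrint loops over the selected builds, skips any flagged ManualyPlaced, and appends each remaining one's class, transform, health, size and interaction state to BuildItemSave.
; It only fills that array, with no disk write or load logic, and an IsASwitch check is left unconnected.
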(fn SaveBluePrint
  (params (Selected%20Builds :type Array%20of%20BP%20Master%20Build%20Object%20References))
  (for _array_element Selected%20Builds
    (if (not (Variables|/Game/DATA/Blueprints/Actors/BuildItems/BP_MasterBuild.BP_MasterBuild_C|GetManualyPlaced _array_element))
      (Utilities|Array|Add (Variables|Default|GetBuildItemSave) (Utilities|Struct|MakeS_BuildItemsSave (Utilities|GetClass _array_element) (Transformation|GetActorTransform _array_element) (Variables|/Game/DATA/Blueprints/Actors/BuildItems/BP_MasterBuild.BP_MasterBuild_C|GetHealth _array_element) (Variables|/Game/DATA/Blueprints/Actors/BuildItems/BP_MasterBuild.BP_MasterBuild_C|GetSize _array_element) (Variables|/Game/DATA/Blueprints/Actors/BuildItems/BP_MasterBuild.BP_MasterBuild_C|GetInteractON _array_element) 0))))
  (return))