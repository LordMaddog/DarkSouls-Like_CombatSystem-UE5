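; BP_SaveSettings is a settings save object that stores sound values in a SoundSettings map keyed by type.
; GetSound looks up the value for a type, and SetSound writes or overwrites it.
; ModifySound adjusts a value relatively by adding a delta to the stored one through those two functions, with no clamping.
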(fn GetSound
  (params (Type :type E_SoundSetings%20Enum :default "NewEnumerator0"))
  (return (.Value (Utilities|Map|Find (Variables|Default|GetSoundSettings) Type))))

(fn SetSound
  (params (Type :type E_SoundSetings%20Enum :default "NewEnumerator0") (Value :type Float%20%28double-precision%29%20%28by%20ref%29))
  (Utilities|Map|Add (Variables|Default|GetSoundSettings) Type Value)
  (return))

(fn ModifySound
  (params (Type :type E_SoundSetings%20Enum :default "NewEnumerator0") (Value :type Float%20%28double-precision%29))
  (CallFunction|SetSound Type (+ (CallFunction|GetSound Type) Value))
  (return))