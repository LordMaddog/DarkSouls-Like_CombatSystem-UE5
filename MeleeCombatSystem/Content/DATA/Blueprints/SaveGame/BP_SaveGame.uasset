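; SaveGame Blueprint storing player XP, skill stats, equipment, dropped items and built structures.
; Experience and SkillStats maps sit behind get/set helpers; ExperienceLoad rebuilds XP from spent totals and resets costs plus movement and weapon levels, while SkillRestAvalibleSkillpoint sets available points to level minus one.
; Save functions flatten flagged dropped items and non-manually-placed builds into structs, recording switches separately with their linked builds' transforms.
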(fn ExperienceLoad
  (bind _enumvalue (|ForEachE_Experience)
    (:LoopBody
      (switch Utilities|FlowControl|Switch|SwitchonE_Experience _enumvalue
        (:NewEnumerator1
          (CallFunction|SetXp "NewEnumerator1" (CallFunction|GetXP "NewEnumerator3")))
        (:NewEnumerator2
          (CallFunction|SetXp "NewEnumerator2" 100))
        (:NewEnumerator3)
        (:NewEnumerator4
          (CallFunction|SetXp "NewEnumerator4" (CallFunction|GetXP "NewEnumerator6")))
        (:NewEnumerator5
          (CallFunction|SetXp "NewEnumerator5" 100))
        (:NewEnumerator6)
        (:NewEnumerator7
          (CallFunction|SetXp "NewEnumerator7" (CallFunction|GetXP "NewEnumerator9")))
        (:NewEnumerator8
          (CallFunction|SetXp "NewEnumerator8" 100))
        (:NewEnumerator9)
        (:NewEnumerator10
          (CallFunction|SetXp "NewEnumerator10" (CallFunction|GetXP "NewEnumerator12")))
        (:NewEnumerator11
          (CallFunction|SetXp "NewEnumerator11" 100))
        (:NewEnumerator12)
        (:NewEnumerator13
          (CallFunction|SetXp "NewEnumerator13" (CallFunction|GetXP "NewEnumerator15")))
        (:NewEnumerator14
          (CallFunction|SetXp "NewEnumerator14" 100))
        (:NewEnumerator15)
        (:NewEnumerator16
          (CallFunction|SetXp "NewEnumerator16" (CallFunction|GetXP "NewEnumerator18")))
        (:NewEnumerator17
          (CallFunction|SetXp "NewEnumerator17" 100))
        (:NewEnumerator18)
        (:NewEnumerator19)
        (:NewEnumerator22
          (CallFunction|SetXp "NewEnumerator22" 200))
        (:NewEnumerator23
          (CallFunction|SetXp "NewEnumerator23" (CallFunction|GetXP "NewEnumerator19")))
        (:NewEnumerator27
          (CallFunction|SetXp "NewEnumerator27" (+ (CallFunction|GetXP "NewEnumerator27") (CallFunction|GetXP "NewEnumerator36"))))
        (:NewEnumerator28
          (CallFunction|SetXp "NewEnumerator28" 100))
        (:NewEnumerator30
          (CallFunction|SetXp "NewEnumerator30" (+ (CallFunction|GetXP "NewEnumerator30") (CallFunction|GetXP "NewEnumerator37"))))
        (:NewEnumerator31
          (CallFunction|SetXp "NewEnumerator31" 10))
        (:NewEnumerator33
          (CallFunction|SetXp "NewEnumerator33" (+ (CallFunction|GetXP "NewEnumerator33") (CallFunction|GetXP "NewEnumerator38"))))
        (:NewEnumerator34
          (CallFunction|SetXp "NewEnumerator34" 50))
        (:NewEnumerator39
          (CallFunction|SetXp "NewEnumerator39" (+ (CallFunction|GetXP "NewEnumerator39") (CallFunction|GetXP "NewEnumerator41"))))
        (:NewEnumerator40
          (CallFunction|SetXp "NewEnumerator40" 10))
        (:NewEnumerator43
          (CallFunction|SetXp "NewEnumerator43" (+ (CallFunction|GetXP "NewEnumerator43") (CallFunction|GetXP "NewEnumerator46"))))
        (:NewEnumerator44
          (CallFunction|SetXp "NewEnumerator44" 10))))
    (:then
      (CallFunction|SetXp "NewEnumerator42" 1)
      (CallFunction|SetXp "NewEnumerator45" 1)
      (CallFunction|SetXp "NewEnumerator35" 1)
      (CallFunction|SetXp "NewEnumerator32" 1)
      (CallFunction|SetXp "NewEnumerator29" 1)
      (return))))

(fn GetXP
  (params (XPType :type E_Experience%20Enum :default "NewEnumerator0"))
  (return (.Value (Utilities|Map|Find (Variables|Default|GetExperience) XPType))))

(fn SetXp
  (params (Stat :type E_Experience%20Enum :default "NewEnumerator22") (Value :type Integer))
  (Utilities|Map|Add (Variables|Default|GetExperience) Stat Value))

(fn ModifyXP
  (params (Stat :type E_Experience%20Enum :default "NewEnumerator0") (Value :type Integer))
  (bind _return_value (CallFunction|GetXP Stat))
  (bind _returnvalue (+ Value _return_value))
  (CallFunction|SetXp Stat (Math|Integer|Clamp(Integer) _returnvalue 0 _returnvalue)))

(fn RemoveSpecialEquipment
  (if (.ReturnValue (Utilities|Map|Find (Variables|Default|GetEquiped) "/Game/DATA/Blueprints/Actors/Armor/BP_HyperArmor.BP_HyperArmor_C"))
    (Utilities|Map|Remove (Variables|Default|GetEquiped) "/Game/DATA/Blueprints/Actors/Armor/BP_HyperArmor.BP_HyperArmor_C"))
  (if (.ReturnValue (Utilities|Map|Find (Variables|Default|GetEquiped) "/Game/DATA/Blueprints/Actors/Useables/BP_IceCrystalItem.BP_IceCrystalItem_C"))
    (Utilities|Map|Remove (Variables|Default|GetEquiped) "/Game/DATA/Blueprints/Actors/Useables/BP_IceCrystalItem.BP_IceCrystalItem_C"))
  (return))

(fn GetSkillStats
  (params (Skill :type Gameplay%20Tag%20Structure))
  (bind _skillstats (Variables|Default|GetSkillStats))
  (bind _value (Utilities|Map|Find _skillstats Skill))
  (return (.manacost _value) (.staminacost _value) (.skillxp _value) (.levelupcost _value) (.skilllevel _value) (.availablepoints _value) (.power _value) (.effectiveness _value) (.type _value)))

(fn SetSkillStat
  (params (Skill :type Gameplay%20Tag%20Structure%20%28by%20ref%29) (Mana%20Cost :type Integer) (Stamina%20Cost :type Integer) (SkillXP :type Integer) (Level%20Up%20Cost :type Integer) (Skill%20Level :type Integer) (Available%20Points :type Integer) (Power :type Float%20%28double-precision%29) (Effectiveness :type Float%20%28double-precision%29) (Type :type E_DamageTypes%20Enum :default "NewEnumerator0"))
  (bind _structout (Utilities|Struct|SetmembersinS_Ability (.Value (Utilities|Map|Find (Variables|Default|GetSkillStats) Skill)) Mana%20Cost Stamina%20Cost SkillXP Level%20Up%20Cost Skill%20Level Available%20Points Power Effectiveness Type))
  (Utilities|Map|Add (Variables|Default|GetSkillStats) Skill _structout))

(fn SkillRestAvalibleSkillpoint
  (bind _keys (Utilities|Map|Keys (Variables|Default|GetSkillStats)))
  (for _array_element _keys
    (CallFunction|SetSkillStat _array_element (.Mana%20Cost (CallFunction|GetSkillStats _array_element)) (.Stamina%20Cost (CallFunction|GetSkillStats _array_element)) (.Skill%20XP (CallFunction|GetSkillStats _array_element)) (.Level%20Up%20Cost (CallFunction|GetSkillStats _array_element)) (.Skill%20Level (CallFunction|GetSkillStats _array_element)) (- (.Skill%20Level (CallFunction|GetSkillStats _array_element)) 1) (.Power (CallFunction|GetSkillStats _array_element)) (.Effectiveness (CallFunction|GetSkillStats _array_element)) (.Type (CallFunction|GetSkillStats _array_element)))))

(fn SaveDroppeditems
  (params (Array :type Array%20of%20BP%20Master%20Item%20Object%20References))
  (Utilities|Array|Clear (Variables|Default|GetSavedDroppedItems))
  (for _array_element Array
    (if (and (Utilities|Enum|Equal(Enum) (Variables|/Game/DATA/Blueprints/Actors/BP_MasterItem.BP_MasterItem_C|GetActiveType _array_element) "NewEnumerator2") (Variables|/Game/DATA/Blueprints/Actors/BP_MasterItem.BP_MasterItem_C|GetShouldSave _array_element))
      (Utilities|Array|Add (Variables|Default|GetSavedDroppedItems) (Utilities|Struct|MakeS_ReSpawnItem (Utilities|GetClass _array_element) (Variables|/Game/DATA/Blueprints/Actors/BP_MasterItem.BP_MasterItem_C|GetItemInfo _array_element) (Variables|/Game/DATA/Blueprints/Actors/BP_MasterItem.BP_MasterItem_C|GetAmount _array_element) (Transformation|GetActorTransform _array_element)))))
  (return))

(fn SaveBuildItems
  (params (Items :type Array%20of%20BP%20Master%20Build%20Object%20References))
  (Utilities|Array|Clear (Variables|Default|GetBuildItemSave))
  (Utilities|Array|Clear (Variables|Default|GetBuildItemSaveSwitch))
  (for _array_element Items
    (if (not (Variables|/Game/DATA/Blueprints/Actors/BuildItems/BP_MasterBuild.BP_MasterBuild_C|GetManualyPlaced _array_element))
      (if (not (Variables|/Game/DATA/Blueprints/Actors/BuildItems/BP_MasterBuild.BP_MasterBuild_C|GetIsASwitch _array_element))
        (Utilities|Array|Add (Variables|Default|GetBuildItemSave) (Utilities|Struct|MakeS_BuildItemsSave (Utilities|GetClass _array_element) (Transformation|GetActorTransform _array_element) (Variables|/Game/DATA/Blueprints/Actors/BuildItems/BP_MasterBuild.BP_MasterBuild_C|GetHealth _array_element) (Variables|/Game/DATA/Blueprints/Actors/BuildItems/BP_MasterBuild.BP_MasterBuild_C|GetSize _array_element) (Variables|/Game/DATA/Blueprints/Actors/BuildItems/BP_MasterBuild.BP_MasterBuild_C|GetInteractON _array_element) (Variables|/Game/DATA/Blueprints/Actors/BuildItems/BP_MasterBuild.BP_MasterBuild_C|GetChangedMat _array_element)))
        (else
          (bind _asbp_base_switch (Utilities|Casting|CastToBP_BaseSwitch _array_element))
          (Utilities|Array|Clear (LocalVariables|GetL_Transfor))
          (for _array_element_2 (Variables|/Game/DATA/Blueprints/Actors/BuildItems/Builds/Base/BP_BaseSwitch.BP_BaseSwitch_C|GetInteractiveBuilds _asbp_base_switch)
            (Utilities|IsValid _array_element_2
              (:Is%20Valid
                (Utilities|Array|Add (LocalVariables|GetL_Transfor) (Transformation|GetWorldTransform (Variables|/Game/DATA/Blueprints/Actors/BuildItems/BP_MasterBuild.BP_MasterBuild_C|GetCollisionCheckMesh _array_element_2))))))
          (Utilities|Array|Add (Variables|Default|GetBuildItemSaveSwitch) (Utilities|Struct|MakeS_BuildItemsSaveSwitch (Utilities|GetClass _asbp_base_switch) (Transformation|GetActorTransform _asbp_base_switch) (Variables|/Game/DATA/Blueprints/Actors/BuildItems/BP_MasterBuild.BP_MasterBuild_C|GetHealth _asbp_base_switch) (Variables|/Game/DATA/Blueprints/Actors/BuildItems/BP_MasterBuild.BP_MasterBuild_C|GetSize _asbp_base_switch) (Variables|/Game/DATA/Blueprints/Actors/BuildItems/BP_MasterBuild.BP_MasterBuild_C|GetInteractON _asbp_base_switch) (LocalVariables|GetL_Transfor) (Variables|/Game/DATA/Blueprints/Actors/BuildItems/BP_MasterBuild.BP_MasterBuild_C|GetChangedMat _asbp_base_switch))))))))