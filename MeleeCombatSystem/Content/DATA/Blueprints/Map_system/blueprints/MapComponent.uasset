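; Map icon component that shows its owning actor on the game's map areas.
; On BeginPlay it loads icon settings from the MapIconPresets data table, then after a delay for map initialization registers with BP_Map_Area actors found by tag, either any active map or active ones in MapsList.
; EndPlay removes the icon.
; A helper can activate a tagged map with the latest W_02_map_image widget, but its event-graph call is unconnected.
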(event Custom|End
  ;[1 1 1] Map component for icons,
  ; Beginplay is here.
  (BasicLogic|UpdateRegister true))

(event EventBeginPlay
  ;[1 1 1] Map component for icons,
  ; Beginplay is here.
  (Utilities|FlowControl|Sequence
    (:then_0
      (BasicLogic|InitDataIcon (Variables|BasicData|Geticon_data)))
    (:then_1
      (Utilities|FlowControl|Delay 3.0) ; delay to let the area map to init.
      (BasicLogic|UpdateRegister (not (Variables|BasicData|Getshow_icon))))))

(event EventEndPlay
  (params (EndPlayReason :type EEndPlayReason%20Enum :default "Destroyed"))
  ;[1 1 1] Map component for icons,
  ; Beginplay is here.
  (BasicLogic|UpdateRegister true))

(fn ActivateMap
  (params (map_id :type Name))
  ;[1 1 1] Activate map for base widget.
  (LocalVariables|Setlocal_map map_id)
  (bind (_is_valid _map_widget) (BasicLogic|GetLayoutWidget))
  (if _is_valid
    (bind _outactors (Actor|GetAllActorswithTag (LocalVariables|Getlocal_map)))
    (if (Utilities|Array|IsValidIndex _outactors)
      (bind _asbp_map_area (Utilities|Casting|CastToBP_Map_Area (Utilities|Array|Get(acopy) _outactors)))
      (Default|SetMap _asbp_map_area true _map_widget))))

(fn GetLayoutWidget
  ;[1 1 1] Get players main widget for map.
  (bind _foundwidgets (Widget|GetAllWidgetsOfClass "/Game/DATA/Blueprints/Map_system/widgets/w_02_map_image.w_02_map_image_C" false))
  (if (Utilities|Array|IsValidIndex _foundwidgets (Utilities|Array|LastIndex _foundwidgets))
    (return (Utilities|Array|IsValidIndex _foundwidgets (Utilities|Array|LastIndex _foundwidgets)) (Utilities|Array|Get(acopy) _foundwidgets (Utilities|Array|LastIndex _foundwidgets)))
    (else
      (return false 0))))

(fn InitDataIcon
  (params (icon_data_id :type Name))
  ;[1 1 1] Use data icon.
  (bind _returnvalue (Utilities|GetDataTableRow "/Game/DATA/Blueprints/Map_system/common/MapIconPresets.MapIconPresets" icon_data_id)
    (:then
      (Variables|BasicData|Seticon_info (Utilities|Struct|Breaks_IconBase _returnvalue)))))

(fn SetIconName
  (params (icon_name :type Name))
  ;[1 1 1] Set icon name.
  (Variables|BasicData|Seticon_name icon_name))

(fn UpdateRegister
  (params (remove_icon :type Boolean))
  ;[1 1 1] Update icon and its value in the specific maps or all of them.
  (if (Variables|BasicData|Getany_map)
    (bind _outactors (Actor|GetAllActorswithTag "dlg_map_active"))
    (for _array_element _outactors
      (bind _asbp_map_area (Utilities|Casting|CastToBP_Map_Area _array_element))
      (Default|RegisterIcon _asbp_map_area (Components|GetOwner) self remove_icon))
    (else
      (for _array_element_2 (Variables|BasicData|Getmaps_list)
        (bind _outactors_2 (Actor|GetAllActorswithTag _array_element_2))
        (for _array_element_3 _outactors_2
          (bind _asbp_map_area_2 (Utilities|Casting|CastToBP_Map_Area _array_element_3))
          (if (Variables|/Game/DATA/Blueprints/Map_system/blueprints/BP_Map_Area.BP_Map_Area_C|Getis_active _asbp_map_area_2)
            (Default|RegisterIcon _asbp_map_area_2 (Components|GetOwner) self remove_icon)))))))