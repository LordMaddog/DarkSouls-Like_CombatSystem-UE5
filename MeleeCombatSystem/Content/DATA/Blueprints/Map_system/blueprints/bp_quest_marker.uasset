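; Generic quest marker that shows quest objectives as icons through the map system's BpDlgMapComponent.
; An init event stores the quest actor, objective ID and sub-objective, sets the icon color, then updates the component's map registration.
; The icon-type switch has no branches, and the color selection runs on constants, so icons always come out red despite green, blue and white options.
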(event Custom|init_quest_icon
  (params (quest_actor :type Actor%20Object%20Reference) (objective_id :type Name) (sub_objective :type Boolean) (icon_type :type Byte :default 0))
  ;[1 1 1] This is generic quest marker for icons.
  ; Beginplay is here.
  (Variables|BasicData|Setquest_actor quest_actor)
  (Variables|BasicData|Setobjective_id objective_id)
  (Variables|BasicData|Setsub_objective sub_objective)
  (Utilities|FlowControl|Sequence
    (:then_0
      (switch Utilities|FlowControl|Switch|Switchon icon_type))
    (:then_1
      (if true
        (switch int 0
          (:0
            (Utilities|Struct|Setmembersins_IconData (Variables|/Game/DATA/Blueprints/Map_system/blueprints/MapComponent.MapComponent_C|Geticon_info (Variables|BasicData|Getbp_dlg_map_component)) "(R=1.000000,G=0.050000,B=0.050000,A=1.000000)"))
          (:1
            (Utilities|Struct|Setmembersins_IconData (Variables|/Game/DATA/Blueprints/Map_system/blueprints/MapComponent.MapComponent_C|Geticon_info (Variables|BasicData|Getbp_dlg_map_component)) "(R=0.050000,G=1.000000,B=0.244333,A=1.000000)"))
          (:2
            (Utilities|Struct|Setmembersins_IconData (Variables|/Game/DATA/Blueprints/Map_system/blueprints/MapComponent.MapComponent_C|Geticon_info (Variables|BasicData|Getbp_dlg_map_component)) "(R=0.050000,G=0.294997,B=1.000000,A=1.000000)")))
        (else
          (Utilities|Struct|Setmembersins_IconData (Variables|/Game/DATA/Blueprints/Map_system/blueprints/MapComponent.MapComponent_C|Geticon_info (Variables|BasicData|Getbp_dlg_map_component)) "(R=1.000000,G=1.000000,B=1.000000,A=1.000000)"))))
    (:then_2
      (Default|UpdateRegister (Variables|BasicData|Getbp_dlg_map_component) true))))

(fn ConstructionScript)