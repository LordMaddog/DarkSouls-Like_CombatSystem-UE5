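; Walled arena trigger that runs a Bullet Heaven survival encounter when the player enters.
; After a short delay it raises walls, adds the player's BulletHeaven component and spawns SpawnEnemiesList waves at traced random points near the player.
; It polls until spawned enemies die, triggers the XP magnet, then wins.
; Winning or leaving drops the walls, animates a score screen through chained timelines and awards XP scaled by performance.
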(event OnComponentBeginOverlap(Box)
  (params (OverlappedComponent :type Primitive%20Component%20Object%20Reference) (OtherActor :type Actor%20Object%20Reference) (OtherComp :type Primitive%20Component%20Object%20Reference) (OtherBodyIndex :type Integer) (bFromSweep :type Boolean) (SweepResult :type Hit%20Result%20Structure%20%28by%20ref%29))
  (bind _isplayer (CallFunction|ToCastorNottoCast OtherActor))
  (if _isplayer
    (Variables|Default|SetActive true)
    (Utilities|FlowControl|Delay 3.0)
    (if (Variables|Default|GetActive)
      (Utilities|Array|Clear (Variables|Default|GetSpawnedActors))
      (Variables|/Game/DATA/BP_PC.BP_PC_C|SetBulletHeavenActive (Variables|Default|GetPlayer) true)
      (CallFunction|SetWallonOff true)
      (CallFunction|SpawnEnemies)
      (bind _returnvalue (AddComponent|AddBulletHeavenComponet (Variables|Default|GetPlayer)))
      (Variables|Default|SetBulletHeavenComponet _returnvalue)
      (Default|Activate (Variables|/Game/DATA/UI/Inventory/WBP_MainWidget.WBP_MainWidget_C|GetCW_BulletXPBar (Variables|/Game/DATA/Blueprints/Actors/Inventory/BP_Inventory.BP_Inventory_C|GetMainWidget (Variables|/Game/DATA/BP_PC.BP_PC_C|GetInventory (Variables|Default|GetPlayer)))))
      (Widget|SetVisibility (Variables|/Game/DATA/UI/Inventory/WBP_MainWidget.WBP_MainWidget_C|GetCW_BulletXPBar (Variables|/Game/DATA/Blueprints/Actors/Inventory/BP_Inventory.BP_Inventory_C|GetMainWidget (Variables|/Game/DATA/BP_PC.BP_PC_C|GetInventory (Variables|Default|GetPlayer)))) "HitTestInvisible"))))

(event OnComponentEndOverlap(Box)
  (params (OverlappedComponent :type Primitive%20Component%20Object%20Reference) (OtherActor :type Actor%20Object%20Reference) (OtherComp :type Primitive%20Component%20Object%20Reference) (OtherBodyIndex :type Integer))
  (bind _isplayer (CallFunction|ToCastorNottoCast OtherActor))
  (if _isplayer
    (if (Variables|Default|GetActive)
      (CallFunction|SetWallonOff false)
      (Variables|Default|SetActive false)
      (Variables|Default|SetIndex 0)
      (CallFunction|Score)
      (bind _bulletheavencomponet (Variables|Default|GetBulletHeavenComponet)
        (:then
          (Default|RemoveSelf _bulletheavencomponet)
          (Variables|/Game/DATA/BP_PC.BP_PC_C|SetBulletHeavenActive (Variables|Default|GetPlayer) false)
          (Default|Activate (Variables|/Game/DATA/UI/Inventory/WBP_MainWidget.WBP_MainWidget_C|GetCW_BulletXPBar (Variables|/Game/DATA/Blueprints/Actors/Inventory/BP_Inventory.BP_Inventory_C|GetMainWidget (Variables|/Game/DATA/BP_PC.BP_PC_C|GetInventory (Variables|Default|GetPlayer)))))
          (Widget|SetVisibility (Variables|/Game/DATA/UI/Inventory/WBP_MainWidget.WBP_MainWidget_C|GetCW_BulletXPBar (Variables|/Game/DATA/Blueprints/Actors/Inventory/BP_Inventory.BP_Inventory_C|GetMainWidget (Variables|/Game/DATA/BP_PC.BP_PC_C|GetInventory (Variables|Default|GetPlayer)))) "Collapsed"))
        (:else)))))

(event Custom|SpawnEnemies
  (if (Variables|Default|GetActive)
    (Variables|Default|SetCurrentTypeSpawned 0)
    (Math|Integer|IncrementInt (Variables|Default|GetIndex)
      (:%20%20
        (bind _delay_to_next_enemy_spawn (CallFunction|SpawnEnemy (Variables|Default|GetIndex)))
        (Utilities|FlowControl|Delay _delay_to_next_enemy_spawn)
        (if (.ReturnValue (Utilities|Map|Find (Variables|Default|GetSpawnEnemiesList) (Variables|Default|GetIndex)))
          (CallFunction|SpawnEnemies)
          (else
            (CallFunction|CheckifAllDead)))))))

(event Custom|CheckIfAllDead
  (if (Variables|Default|GetActive)
    (if (> (Utilities|Array|Length (Variables|Default|GetSpawnedActors)) 0)
      (Utilities|FlowControl|Delay 1.0)
      (for (_array_element _array_index) (Variables|Default|GetSpawnedActors)
        (Utilities|IsValid _array_element
          (:Is%20Valid
            (bind _asbp_pc (Utilities|Casting|CastToBP_PC _array_element))
            (if (Variables|/Game/DATA/Blueprints/Components/CombatComponent.CombatComponent_C|GetDead (Variables|/Game/DATA/BP_PC.BP_PC_C|GetCombatComponent _asbp_pc))
              (Utilities|Array|RemoveIndex (Variables|Default|GetSpawnedActors) _array_index)))
          (:Is%20Not%20Valid
            (Utilities|Array|RemoveIndex (Variables|Default|GetSpawnedActors) _array_index))))
      (CallFunction|CheckifAllDead)
      (else
        (Default|Magnet (Variables|Default|GetBulletHeavenComponet))
        (Utilities|FlowControl|Delay 1e+01)
        (CallFunction|Win)))))

(event Custom|Win
  (CallFunction|SetWallonOff false)
  (Variables|Default|SetActive false)
  (Variables|Default|SetIndex 0)
  (CallFunction|Score)
  (bind _bulletheavencomponet (Variables|Default|GetBulletHeavenComponet)
    (:then
      (Default|RemoveSelf _bulletheavencomponet)
      (Variables|/Game/DATA/BP_PC.BP_PC_C|SetBulletHeavenActive (Variables|Default|GetPlayer) false)
      (Default|Activate (Variables|/Game/DATA/UI/Inventory/WBP_MainWidget.WBP_MainWidget_C|GetCW_BulletXPBar (Variables|/Game/DATA/Blueprints/Actors/Inventory/BP_Inventory.BP_Inventory_C|GetMainWidget (Variables|/Game/DATA/BP_PC.BP_PC_C|GetInventory (Variables|Default|GetPlayer)))))
      (Widget|SetVisibility (Variables|/Game/DATA/UI/Inventory/WBP_MainWidget.WBP_MainWidget_C|GetCW_BulletXPBar (Variables|/Game/DATA/Blueprints/Actors/Inventory/BP_Inventory.BP_Inventory_C|GetMainWidget (Variables|/Game/DATA/BP_PC.BP_PC_C|GetInventory (Variables|Default|GetPlayer)))) "Collapsed"))
    (:else)))

(event EventBeginPlay
  (CallFunction|SetWallonOff false))

(event Collision|EventActorBeginOverlap
  (params (OtherActor :type Actor%20Object%20Reference)))

(event EventTick
  (params (DeltaSeconds :type Float%20%28single-precision%29)))

(event EventAddCharacter
  (params (CharacterIn :type Actor%20Object%20Reference))
  (Utilities|Array|Add (Variables|Default|GetSpawnedActors) CharacterIn))

(event Custom|Scrolling%20Numbers
  (bind _player (Variables|Default|GetPlayer))
  (bind _player_2 (Variables|Default|GetPlayer))
  (bind _player_3 (Variables|Default|GetPlayer))
  (bind _player_4 (Variables|Default|GetPlayer))
  (bind _player_5 (Variables|Default|GetPlayer))
  (bind _player_6 (Variables|Default|GetPlayer))
  (bind _inventory (Variables|/Game/DATA/BP_PC.BP_PC_C|GetInventory _player))
  (bind _inventory_2 (Variables|/Game/DATA/BP_PC.BP_PC_C|GetInventory _player_2))
  (bind _inventory_3 (Variables|/Game/DATA/BP_PC.BP_PC_C|GetInventory _player_3))
  (bind _inventory_4 (Variables|/Game/DATA/BP_PC.BP_PC_C|GetInventory _player_4))
  (bind _inventory_5 (Variables|/Game/DATA/BP_PC.BP_PC_C|GetInventory _player_5))
  (bind _inventory_6 (Variables|/Game/DATA/BP_PC.BP_PC_C|GetInventory _player_6))
  (bind _mainwidget (Variables|/Game/DATA/Blueprints/Actors/Inventory/BP_Inventory.BP_Inventory_C|GetMainWidget _inventory))
  (bind _mainwidget_2 (Variables|/Game/DATA/Blueprints/Actors/Inventory/BP_Inventory.BP_Inventory_C|GetMainWidget _inventory_2))
  (bind _mainwidget_3 (Variables|/Game/DATA/Blueprints/Actors/Inventory/BP_Inventory.BP_Inventory_C|GetMainWidget _inventory_3))
  (bind _mainwidget_4 (Variables|/Game/DATA/Blueprints/Actors/Inventory/BP_Inventory.BP_Inventory_C|GetMainWidget _inventory_4))
  (bind _mainwidget_5 (Variables|/Game/DATA/Blueprints/Actors/Inventory/BP_Inventory.BP_Inventory_C|GetMainWidget _inventory_5))
  (bind _mainwidget_6 (Variables|/Game/DATA/Blueprints/Actors/Inventory/BP_Inventory.BP_Inventory_C|GetMainWidget _inventory_6))
  (bind _cw_scorescreen (Variables|/Game/DATA/UI/Inventory/WBP_MainWidget.WBP_MainWidget_C|GetCW_ScoreScreen _mainwidget))
  (bind _cw_scorescreen_2 (Variables|/Game/DATA/UI/Inventory/WBP_MainWidget.WBP_MainWidget_C|GetCW_ScoreScreen _mainwidget_2))
  (bind _cw_scorescreen_3 (Variables|/Game/DATA/UI/Inventory/WBP_MainWidget.WBP_MainWidget_C|GetCW_ScoreScreen _mainwidget_3))
  (bind _cw_scorescreen_4 (Variables|/Game/DATA/UI/Inventory/WBP_MainWidget.WBP_MainWidget_C|GetCW_ScoreScreen _mainwidget_4))
  (bind _cw_scorescreen_5 (Variables|/Game/DATA/UI/Inventory/WBP_MainWidget.WBP_MainWidget_C|GetCW_ScoreScreen _mainwidget_5))
  (bind _cw_scorescreen_6 (Variables|/Game/DATA/UI/Inventory/WBP_MainWidget.WBP_MainWidget_C|GetCW_ScoreScreen _mainwidget_6))
  (bind _newtrack_0 (Timeline|Timeline PlayFromStart)
    (:Update
      (Rendering|Components|TextRender|SetText (Variables|/Game/DATA/UI/BulletHeaven/CW_ScoreScreen.CW_ScoreScreen_C|GetAmountOfKills _cw_scorescreen) (Utilities|Text|ToText(Integer) (Math|Float|Floor (Math|Float|Lerp 0.0 (Math|Conversions|ToFloat(Integer) (Variables|Default|GetKills)) _newtrack_0))))
      (Rendering|Components|TextRender|SetText (Variables|/Game/DATA/UI/BulletHeaven/CW_ScoreScreen.CW_ScoreScreen_C|GetKillsScoreMultiplier _cw_scorescreen) (Utilities|Text|ToText(Float) (* (Math|Float|Lerp 0.0 (Math|Conversions|ToFloat(Integer) (Variables|Default|GetKills)) _newtrack_0) 0.01) "HalfToEven"))
      (Audio|PlaySoundatLocation (Variables|Default|GetScoreScrolSound) (Transformation|GetWorldLocation (Variables|/Script/Engine.Character|GetMesh (Variables|Default|GetPlayer))) "0, 0, 0" (+ _newtrack_0 1.0) 1.0 0.0 0 0 0 0))
    (:Finished
      (bind _newtrack_0_2 (Timeline|Timeline_0 PlayFromStart)
        (:Update
          (Rendering|Components|TextRender|SetText (Variables|/Game/DATA/UI/BulletHeaven/CW_ScoreScreen.CW_ScoreScreen_C|GetMaxCombo _cw_scorescreen_2) (Utilities|Text|ToText(Integer) (Math|Float|Floor (Math|Float|Lerp 0.0 (Variables|Default|GetCombo) _newtrack_0_2))))
          (Rendering|Components|TextRender|SetText (Variables|/Game/DATA/UI/BulletHeaven/CW_ScoreScreen.CW_ScoreScreen_C|GetComboScoreMultiplier _cw_scorescreen_2) (Utilities|Text|ToText(Float) (* (Math|Float|Lerp 0.0 (Variables|Default|GetCombo) _newtrack_0_2) 0.01) "HalfToEven"))
          (Audio|PlaySoundatLocation (Variables|Default|GetScoreScrolSound) (Transformation|GetWorldLocation (Variables|/Script/Engine.Character|GetMesh (Variables|Default|GetPlayer))) "0, 0, 0" (+ _newtrack_0_2 1.0) 1.0 0.0 0 0 0 0))
        (:Finished
          (bind _newtrack_0_3 (Timeline|Timeline_1 PlayFromStart)
            (:Update
              (Rendering|Components|TextRender|SetText (Variables|/Game/DATA/UI/BulletHeaven/CW_ScoreScreen.CW_ScoreScreen_C|GetDamageDealtScore _cw_scorescreen_3) (Utilities|Text|ToText(Integer) (Math|Float|Floor (Math|Float|Lerp 0.0 (Math|Conversions|ToFloat(Integer) (Variables|Default|GetDamage%20Dealt)) _newtrack_0_3))))
              (Rendering|Components|TextRender|SetText (Variables|/Game/DATA/UI/BulletHeaven/CW_ScoreScreen.CW_ScoreScreen_C|GetDamageDealtScoreMultiplier _cw_scorescreen_3) (Utilities|Text|ToText(Float) (* (Math|Float|Lerp 0.0 (Math|Conversions|ToFloat(Integer) (Variables|Default|GetDamage%20Dealt)) _newtrack_0_3) 0.001) "HalfToEven"))
              (Audio|PlaySoundatLocation (Variables|Default|GetScoreScrolSound) (Transformation|GetWorldLocation (Variables|/Script/Engine.Character|GetMesh (Variables|Default|GetPlayer))) "0, 0, 0" (+ _newtrack_0_3 1.0) 1.0 0.0 0 0 0 0))
            (:Finished
              (bind _newtrack_0_4 (Timeline|Timeline_2 PlayFromStart)
                (:Update
                  (Rendering|Components|TextRender|SetText (Variables|/Game/DATA/UI/BulletHeaven/CW_ScoreScreen.CW_ScoreScreen_C|GetDamageReceivedScore _cw_scorescreen_4) (Utilities|Text|ToText(Integer) (Math|Float|Floor (Math|Float|Lerp 0.0 (Math|Conversions|ToFloat(Integer) (Variables|Default|GetDamage%20Received)) _newtrack_0_4))))
                  (Rendering|Components|TextRender|SetText (Variables|/Game/DATA/UI/BulletHeaven/CW_ScoreScreen.CW_ScoreScreen_C|GetDamageReceivedScoreMultiplier _cw_scorescreen_4) (Utilities|Text|ToText(Float) (* (* (Math|Float|Lerp 0.0 (Math|Conversions|ToFloat(Integer) (Variables|Default|GetDamage%20Received)) _newtrack_0_4) 0.01) -1.0) "HalfToEven"))
                  (Audio|PlaySoundatLocation (Variables|Default|GetScoreScrolSound) (Transformation|GetWorldLocation (Variables|/Script/Engine.Character|GetMesh (Variables|Default|GetPlayer))) "0, 0, 0" (+ _newtrack_0_4 1.0) 1.0 0.0 0 0 0 0))
                (:Finished
                  (bind _newtrack_0_5 (Timeline|Timeline_3 PlayFromStart)
                    (:Update
                      (Rendering|Components|TextRender|SetText (Variables|/Game/DATA/UI/BulletHeaven/CW_ScoreScreen.CW_ScoreScreen_C|GetDamageHealedScore _cw_scorescreen_5) (Utilities|Text|ToText(Integer) (Math|Float|Floor (Math|Float|Lerp 0.0 (Math|Conversions|ToFloat(Integer) (Variables|Default|GetDamage%20Healed)) _newtrack_0_5))))
                      (Rendering|Components|TextRender|SetText (Variables|/Game/DATA/UI/BulletHeaven/CW_ScoreScreen.CW_ScoreScreen_C|GetDamageHealedScoreMultiplier _cw_scorescreen_5) (Utilities|Text|ToText(Float) (* (Math|Float|Lerp 0.0 (Math|Conversions|ToFloat(Integer) (Variables|Default|GetDamage%20Healed)) _newtrack_0_5) 0.01) "HalfToEven"))
                      (Audio|PlaySoundatLocation (Variables|Default|GetScoreScrolSound) (Transformation|GetWorldLocation (Variables|/Script/Engine.Character|GetMesh (Variables|Default|GetPlayer))) "0, 0, 0" (+ _newtrack_0_5 1.0) 1.0 0.0 0 0 0 0))
                    (:Finished
                      (bind _newtrack_0_6 (Timeline|Timeline_4 PlayFromStart)
                        (:Update
                          (Rendering|Components|TextRender|SetText (Variables|/Game/DATA/UI/BulletHeaven/CW_ScoreScreen.CW_ScoreScreen_C|GetAmountOfXPGained _cw_scorescreen_6) (Utilities|Text|ToText(Integer) (Math|Float|Floor (Math|Float|Lerp 0.0 (Variables|Default|GetTotal%20XP%20Gained) _newtrack_0_6))))
                          (Rendering|Components|TextRender|SetText (Variables|/Game/DATA/UI/BulletHeaven/CW_ScoreScreen.CW_ScoreScreen_C|GetDefaultMultiplier _cw_scorescreen_6) (Utilities|Text|ToText(Float) (Math|Float|Lerp 0.0 0.5 _newtrack_0_6) "HalfToEven"))
                          (Audio|PlaySoundatLocation (Variables|Default|GetScoreScrolSound) (Transformation|GetWorldLocation (Variables|/Script/Engine.Character|GetMesh (Variables|Default|GetPlayer))) "0, 0, 0" (+ _newtrack_0_6 1.0) 1.0 0.0 0 0 0 0))
                        (:Finished
                          (bind _newtrack_0_7 (Timeline|Timeline_5 PlayFromStart)
                            (:Update
                              (Rendering|Components|TextRender|SetText (Variables|/Game/DATA/UI/BulletHeaven/CW_ScoreScreen.CW_ScoreScreen_C|GetTotalMultiplier (Variables|/Game/DATA/UI/Inventory/WBP_MainWidget.WBP_MainWidget_C|GetCW_ScoreScreen (Variables|/Game/DATA/Blueprints/Actors/Inventory/BP_Inventory.BP_Inventory_C|GetMainWidget (Variables|/Game/DATA/BP_PC.BP_PC_C|GetInventory (Variables|Default|GetPlayer))))) (Utilities|Text|ToText(Float) (Math|Float|Lerp 0.0 (Variables|Default|GetXPToGiveMultiplier) _newtrack_0_7) "HalfToEven"))
                              (Audio|PlaySoundatLocation (Variables|Default|GetScoreScrolSound) (Transformation|GetWorldLocation (Variables|/Script/Engine.Character|GetMesh (Variables|Default|GetPlayer))) "0, 0, 0" (+ _newtrack_0_7 1.0) 1.0 0.0 0 0 0 0))
                            (:Finished
                              (bind _newtrack_0_8 (Timeline|Timeline_6 PlayFromStart)
                                (:Update
                                  (Rendering|Components|TextRender|SetText (Variables|/Game/DATA/UI/BulletHeaven/CW_ScoreScreen.CW_ScoreScreen_C|GetFinialScore (Variables|/Game/DATA/UI/Inventory/WBP_MainWidget.WBP_MainWidget_C|GetCW_ScoreScreen (Variables|/Game/DATA/Blueprints/Actors/Inventory/BP_Inventory.BP_Inventory_C|GetMainWidget (Variables|/Game/DATA/BP_PC.BP_PC_C|GetInventory (Variables|Default|GetPlayer))))) (Utilities|Text|ToText(Integer) (Math|Float|Floor (Math|Float|Lerp 0.0 (Math|Conversions|ToFloat(Integer) (Variables|Default|GetXPToGive)) _newtrack_0_8))))
                                  (Audio|PlaySoundatLocation (Variables|Default|GetScoreScrolSound) (Transformation|GetWorldLocation (Variables|/Script/Engine.Character|GetMesh (Variables|Default|GetPlayer))) "0, 0, 0" (+ _newtrack_0_8 1.0) 1.0 0.0 0 0 0 0))
                                (:Finished
                                  (Default|ModifyXP (Variables|/Game/DATA/BP_PC.BP_PC_C|GetStatsComponent (Variables|Default|GetPlayer)) "NewEnumerator0" (Variables|Default|GetXPToGive)))))))))))))))))))

(event Custom|Score
  (Variables|Default|SetCombo 0.0)
  (Variables|Default|SetKills 0)
  (Variables|Default|SetDamage%20Dealt 0)
  (Variables|Default|SetDamage%20Received 0)
  (Variables|Default|SetDamage%20Healed 0)
  (Variables|Default|SetTotal%20XP%20Gained 0.0)
  (bind (_combo _kills _damagedealt _damagereceived _damagehealed _totalxp) (Default|GetScoreStats (Variables|Default|GetBulletHeavenComponet)))
  (Variables|Default|SetCombo _combo)
  (Variables|Default|SetKills _kills)
  (Variables|Default|SetDamage%20Dealt _damagedealt)
  (Variables|Default|SetDamage%20Received _damagereceived)
  (Variables|Default|SetDamage%20Healed _damagehealed)
  (Variables|Default|SetTotal%20XP%20Gained _totalxp)
  (Widget|SetVisibility (Variables|/Game/DATA/UI/Inventory/WBP_MainWidget.WBP_MainWidget_C|GetCW_ScoreScreen (Variables|/Game/DATA/Blueprints/Actors/Inventory/BP_Inventory.BP_Inventory_C|GetMainWidget (Variables|/Game/DATA/BP_PC.BP_PC_C|GetInventory (Variables|Default|GetPlayer)))) "Visible")
  (Variables|Default|SetXPToGiveMultiplier (+ (* (Variables|Default|GetKills) 0.01) (* (Variables|Default|GetCombo) 0.01) (* (Variables|Default|GetDamage%20Dealt) 0.001) (* (* (Variables|Default|GetDamage%20Received) -1) 0.01) (* (Variables|Default|GetDamage%20Healed) 0.01) 0.5))
  (Variables|Default|SetXPToGive (Math|Float|Truncate (* (Variables|Default|GetTotal%20XP%20Gained) (Variables|Default|GetXPToGiveMultiplier))))
  (CallFunction|ScrollingNumbers)
  (Class|CombatBPI|ToggleMouseCursor(Message) (Variables|/Game/DATA/BP_PC.BP_PC_C|GetPlayer%20Controller (Variables|Default|GetPlayer))))

(fn ConstructionScript)

(fn ToCastorNottoCast
  (params (InActor :type Actor%20Object%20Reference))
  (Utilities|IsValid (Variables|Default|GetPlayer)
    (:Is%20Valid
      (if (== (Variables|Default|GetPlayer) InActor)
        _
        (else
          (return false))))
    (:Is%20Not%20Valid
      (bind _asbp_pc (Utilities|Casting|CastToBP_PC InActor)
        (:then
          (if (Variables|/Game/DATA/Blueprints/Components/CombatComponent.CombatComponent_C|GetIsPlayer (Variables|/Game/DATA/BP_PC.BP_PC_C|GetCombatComponent _asbp_pc))
            (Variables|Default|SetPlayer _asbp_pc)
            (else
              (return false))))
        (:CastFailed
          (return false)))))
  (return true))

(fn SpawnEnemy
  (params (Index :type Integer))
  (bind (_loc _rot) (CallFunction|CalculateSpawnLoc))
  (bind _spawnenemieslist (Variables|Default|GetSpawnEnemiesList))
  (bind _value (Utilities|Map|Find _spawnenemieslist Index))
  (if (not (Variables|/Game/DATA/Blueprints/Components/CombatComponent.CombatComponent_C|GetDead (Variables|/Game/DATA/BP_PC.BP_PC_C|GetCombatComponent (Variables|Default|GetPlayer))))
    (bind _returnvalue (Game|SpawnActorfromClass "/Game/DATA/Blueprints/Actors/Utility/BP_SpawnActors.BP_SpawnActors_C" (Math|Transform|MakeTransform _loc (Math|Rotator|MakeRotator 0.0 0.0 (.yaw _rot)) (Math|Conversions|ToVector(Float) (.npcsize _value))) "Undefined" "MultiplyWithRoot" 0 (.startingequipment _value) (.npcclass _value) (.desiredlvl _value) (.npcname _value) (.changename? _value) (.changeclass? _value) (.changeequipment? _value) (.changebht? _value) (.behabiortree _value) (.patrolpoints _value) true false true self 0))
    (Variables|/Game/DATA/Blueprints/Actors/Utility/BP_SpawnActors.BP_SpawnActors_C|SetClass _returnvalue (.npc _value))
    (bind _result (Math|Integer|IncrementInt (Variables|Default|GetCurrentTypeSpawned))
      (:%20%20
        (if (>= _result (.numbertospawn _value))
          (return (.delaytonextenemyspawn _value))
          (else
            (CallFunction|SpawnEnemy Index)))))))

(fn CalculateSpawnLoc
  (bind _returnvalue (Math|Random|RandomFloatinRange 1.5e+03 2.5e+03))
  (bind _box (Variables|Default|GetBox))
  (bind _box_2 (Variables|Default|GetBox))
  (bind _box_3 (Variables|Default|GetBox))
  (bind _player (Variables|Default|GetPlayer))
  (bind _box_4 (Variables|Default|GetBox))
  (bind _minspawndistancefromwall (LocalVariables|GetMinSpawnDistanceFromWall))
  (bind _box_5 (Variables|Default|GetBox))
  (bind _minspawndistancefromwall_2 (LocalVariables|GetMinSpawnDistanceFromWall))
  (bind _returnvalue_2 (Components|Box|GetScaledBoxExtent _box))
  (bind _returnvalue_3 (Transformation|GetWorldLocation _box_2))
  (bind _returnvalue_4 (Transformation|GetWorldLocation _box))
  (bind _returnvalue_5 (Math|Conversions|ToVector(Float) _returnvalue))
  (bind _returnvalue_6 (Transformation|GetActorLocation _player))
  (bind _returnvalue_7 (Components|Box|GetScaledBoxExtent _box_4))
  (bind _returnvalue_8 (Transformation|GetWorldLocation _box_4))
  (bind _returnvalue_9 (Components|Box|GetScaledBoxExtent _box_2))
  (bind _returnvalue_10 (Math|Random|RandomPointinBoundingBox _returnvalue_6 _returnvalue_5))
  (bind _returnvalue_11 (- (.x _returnvalue_4) (.x _returnvalue_2)))
  (bind _returnvalue_12 (- (.y _returnvalue_4) (.y _returnvalue_2)))
  (bind _returnvalue_13 (+ (.x _returnvalue_8) (.x _returnvalue_7)))
  (bind _returnvalue_14 (+ (.y _returnvalue_8) (.y _returnvalue_7)))
  (bind _returnvalue_15 (+ (.z _returnvalue_8) (.z _returnvalue_7)))
  (bind _returnvalue_16 (- (.z _returnvalue_4) (.z _returnvalue_2)))
  (bind _returnvalue_17 (Math|Geometry|IsPointinBox _returnvalue_10 _returnvalue_3 _returnvalue_9))
  (bind (_x _y _z) (Class|KismetMathLibrary|BreakVector3f _returnvalue_10))
  (bind _returnvalue_18 (+ _returnvalue_16 _minspawndistancefromwall))
  (bind _returnvalue_19 (+ _returnvalue_11 _minspawndistancefromwall))
  (bind _returnvalue_20 (+ _returnvalue_12 _minspawndistancefromwall))
  (bind _returnvalue_21 (- _returnvalue_13 _minspawndistancefromwall_2))
  (bind _returnvalue_22 (- _returnvalue_15 _minspawndistancefromwall_2))
  (bind _returnvalue_23 (- _returnvalue_14 _minspawndistancefromwall_2))
  (bind _returnvalue_24 (> _z _returnvalue_22))
  (bind _returnvalue_25 (> _x _returnvalue_21))
  (bind _returnvalue_26 (> _y _returnvalue_23))
  (bind _returnvalue_27 (select _returnvalue_25 _returnvalue_21 _x))
  (bind _returnvalue_28 (select _returnvalue_26 _returnvalue_23 _y))
  (bind _returnvalue_29 (select _returnvalue_24 _returnvalue_22 _z))
  (bind _returnvalue_30 (< _returnvalue_29 _returnvalue_18))
  (bind _returnvalue_31 (< _returnvalue_27 _returnvalue_19))
  (bind _returnvalue_32 (< _returnvalue_28 _returnvalue_20))
  (bind _returnvalue_33 (select _returnvalue_30 _returnvalue_18 _returnvalue_29))
  (bind _returnvalue_34 (select _returnvalue_31 _returnvalue_19 _returnvalue_27))
  (bind _returnvalue_35 (select _returnvalue_32 _returnvalue_20 _returnvalue_28))
  (bind _returnvalue_36 (select _returnvalue_17 _returnvalue_10 (Math|Vector|MakeVector _returnvalue_34 _returnvalue_35 _returnvalue_33)))
  (bind (_outhit _returnvalue_37) (Collision|SphereTraceByChannel (+ _returnvalue_36 (Math|Vector|MakeVector 0.0 0.0 (+ (.z (Transformation|GetWorldLocation _box_3)) (.z (Components|Box|GetScaledBoxExtent _box_3))))) (+ _returnvalue_36 (Math|Vector|MakeVector 0.0 0.0 (- (.z (Transformation|GetWorldLocation _box_5)) (.z (Components|Box|GetScaledBoxExtent _box_5))))) 4e+01 "TraceTypeQuery1" false 0 "ForDuration"))
  (return (select _returnvalue_37 (+ (.ImpactPoint (Collision|BreakHitResult _outhit)) "0.000000,0.000000,300.000000") (.TraceEnd (Collision|BreakHitResult _outhit))) (Math|Rotator|FindLookatRotation (select _returnvalue_37 (+ (.ImpactPoint (Collision|BreakHitResult _outhit)) "0.000000,0.000000,300.000000") (.TraceEnd (Collision|BreakHitResult _outhit))) (Transformation|GetActorLocation (Variables|Default|GetPlayer)))))

(fn SetWallonOff
  (params (OnOff :type Boolean))
  (bind _southwall (Variables|Default|GetSouthWall))
  (bind _southwall_2 (Variables|Default|GetSouthWall))
  (if OnOff
    (Rendering|SetVisibility _southwall_2 true false)
    (Collision|SetCollisionEnabled _southwall_2 "QueryAndPhysics")
    (else
      (Rendering|SetVisibility _southwall false false)
      (Collision|SetCollisionEnabled _southwall "NoCollision"))))

(fn TallyScore
  (params (TargetScore :type Text%20Block%20Object%20Reference) (TargetMultiplyer :type Text%20Block%20Object%20Reference) (MainStat :type Float%20%28double-precision%29) (Alpha :type Float%20%28double-precision%29) (Multiplier :type Float%20%28double-precision%29))
  (bind _returnvalue (Math|Float|Lerp 0.0 MainStat Alpha))
  (Rendering|Components|TextRender|SetText TargetScore (Utilities|Text|ToText(Integer) (Math|Float|Floor _returnvalue)))
  (Rendering|Components|TextRender|SetText TargetMultiplyer (Utilities|Text|ToText(Float) (* _returnvalue Multiplier) "HalfToEven"))
  (Audio|PlaySoundatLocation (Variables|Default|GetScoreScrolSound) (Transformation|GetWorldLocation (Variables|/Script/Engine.Character|GetMesh (Variables|Default|GetPlayer))) "0, 0, 0" (+ Alpha 1.0) 1.0 0.0 0 0 0 0))