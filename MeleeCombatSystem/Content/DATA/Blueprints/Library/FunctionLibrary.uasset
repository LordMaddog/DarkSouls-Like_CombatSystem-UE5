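; Blueprint function library that shows floating damage or healing numbers at a world location through Niagara.
; MakeFloatingNumbers splits the amount into characters and spawns one damage or healing system per character, scaled by size and yawed to player 0's control rotation.
; Each system is offset sideways and gets its glyph via the User.Digit texture override, with the minus sign blanked for damage.
; SpawnDecal is an empty stub.
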(fn MakeFloatingNumbers
  (params (Location :type Vector) (DamageAmount :type Integer) (NumberSize :type Float%20%28double-precision%29) (Damage? :type Boolean))
  (for _array_element (Utilities|String|GetCharacterArrayfromString (Utilities|String|ToString(Integer) DamageAmount))
    (bind _returnvalue (Niagara|SpawnSystematLocation 0 (select Damage? "/Game/DATA/Effects/N_FloatingNumbers.N_FloatingNumbers" "/Game/DATA/Effects/N_FloatingNumbersHealing.N_FloatingNumbersHealing") Location (Math|Rotator|MakeRotator 0.0 1.8e+02 (.yaw (Pawn|GetControlRotation (Game|GetPlayerController 0) :!class /Script/Engine.Controller))) (Math|Conversions|ToVector(Float) NumberSize)))
    (bind _output_get (LocalVariables|SetDigitSystem _returnvalue))
    (Transformation|AddLocalOffset _output_get (Math|Vector|MakeVector 0.0 (LocalVariables|GetTextOffset) 0.0) false false)
    (LocalVariables|SetTextOffset (+ (LocalVariables|GetTextOffset) 25.0))
    (switch string _array_element
      (:1
        (Niagara|SetTextureObject (LocalVariables|GetDigitSystem) "User.Digit" "/Game/DATA/UI/Numbers/1.1"))
      (:2
        (Niagara|SetTextureObject (LocalVariables|GetDigitSystem) "User.Digit" "/Game/DATA/UI/Numbers/2.2"))
      (:3
        (Niagara|SetTextureObject (LocalVariables|GetDigitSystem) "User.Digit" "/Game/DATA/UI/Numbers/3.3"))
      (:4
        (Niagara|SetTextureObject (LocalVariables|GetDigitSystem) "User.Digit" "/Game/DATA/UI/Numbers/4.4"))
      (:5
        (Niagara|SetTextureObject (LocalVariables|GetDigitSystem) "User.Digit" "/Game/DATA/UI/Numbers/5.5"))
      (:6
        (Niagara|SetTextureObject (LocalVariables|GetDigitSystem) "User.Digit" "/Game/DATA/UI/Numbers/6.6"))
      (:7
        (Niagara|SetTextureObject (LocalVariables|GetDigitSystem) "User.Digit" "/Game/DATA/UI/Numbers/7.7"))
      (:8
        (Niagara|SetTextureObject (LocalVariables|GetDigitSystem) "User.Digit" "/Game/DATA/UI/Numbers/8.8"))
      (:9
        (Niagara|SetTextureObject (LocalVariables|GetDigitSystem) "User.Digit" "/Game/DATA/UI/Numbers/9.9"))
      (:0
        (Niagara|SetTextureObject (LocalVariables|GetDigitSystem) "User.Digit" "/Game/DATA/UI/Numbers/0.0"))
      (:-
        (if (not Damage?)
          (Niagara|SetTextureObject (LocalVariables|GetDigitSystem) "User.Digit" "/Game/DATA/UI/Numbers/+.+")
          (else
            (Niagara|SetTextureObject (LocalVariables|GetDigitSystem) "User.Digit" "/Game/DATA/UI/Numbers/+Empty.+Empty")))))))

(fn SpawnDecal
  (params (In%20Hit%20info :type Hit%20Result%20Structure)))