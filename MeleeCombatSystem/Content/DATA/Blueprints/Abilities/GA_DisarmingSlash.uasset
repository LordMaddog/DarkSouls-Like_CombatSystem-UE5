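; Melee skill ability that performs a slash and force-drops equipped items of one equip type from the target hit.
; On start it checks stamina, mana and combat state, turns to target, and polls briefly for the weapon to be drawn.
; It then applies skill damage, poise, hyper armor and costs and plays the attack montage.
; ActivateComboSkill, fired by anim notify, sphere-traces forward, unequips matching items and clears hyper armor on a hit.
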(event EventBeginPlay
  (|CallParentFunction) ; This node is disabled and will not be called.\nDrag off pins to build functionality.
)

(event Collision|EventActorBeginOverlap
  (params (OtherActor :type Actor%20Object%20Reference)))

(event EventTick
  (params (DeltaSeconds :type Float%20%28single-precision%29)))

(event EventGAStart
  (bind _skill (Variables|Default|GetSkill))
  (bind _stats_component (Variables|Default|GetStats%20Component))
  (bind _skill_2 (Variables|Default|GetSkill))
  (bind _skill_3 (Variables|Default|GetSkill))
  (bind _stats_component_2 (Variables|Default|GetStats%20Component))
  (bind _stats_component_3 (Variables|Default|GetStats%20Component))
  (bind _stats_component_4 (Variables|Default|GetStats%20Component))
  (bind (_combat_types _mana_cost _stamina_cost) (Default|GetSkillStats _stats_component_4 _skill_3))
  (bind (_combat_types_2 _mana_cost_2 _stamina_cost_2) (Default|GetSkillStats _stats_component_2 _skill))
  (bind (_combat_types_3 _mana_cost_3 _stamina_cost_3 _skill_xp _level_up_cost _skill_xpspent _skill_level _available_points _power _effectiveness) (Default|GetSkillStats _stats_component_3 _skill_2))
  ;[1 1 1] Slash
  (CallFunction|FloatWeapon false "NewEnumerator2" "NewEnumerator0")
  (if (Math|Boolean|ANDBoolean (Default|StatGreaterThen _stats_component "NewEnumerator2" (Math|Conversions|ToFloat(Integer) _stamina_cost_2)) (Default|StatGreaterThen _stats_component "NewEnumerator4" (Math|Conversions|ToFloat(Integer) _mana_cost_2)) (Default|CanProformCombat (Variables|Default|GetCombat%20Component)))
    (Default|RotatetoTarget (Variables|Default|GetCharacter))
    (Utilities|IsCombatReady?
      (:Exit
        (bind _output_get (Default|SetMeleeSkillUsed (Default|GetMainWeapon (Variables|/Game/DATA/BP_PC.BP_PC_C|GetCombatComponent (Variables|Default|GetCharacter))) (Variables|Default|GetSkill)))
        (Default|SetActionDamageMultiplyer (Default|GetMainWeapon (Variables|/Game/DATA/BP_PC.BP_PC_C|GetCombatComponent (Variables|Default|GetCharacter))) _output_get _power _effectiveness)
        (CallFunction|EquipHyperArmor)
        (Default|PerformComboAction (Variables|Default|GetCombat%20Component) false (Variables|Default|GetAttackMontages))
        (Default|SetState (Variables|Default|GetCombat%20Component) "(TagName=\"Character.State.GenralActionState\")")
        (Default|SetActionCost (Variables|Default|GetStats%20Component) (Variables|Default|GetSkill) (Math|Conversions|ToFloat(Integer) _stamina_cost) (Math|Conversions|ToFloat(Integer) _mana_cost))
        (Default|SetCurrentAction (Variables|Default|GetCombat%20Component) (Variables|Default|GetSkill))
        (CallFunction|Done 3.0)))
    (else
      (Default|OOMCheck (Variables|Default|GetStats%20Component) (Math|Conversions|ToFloat(Integer) (.Stamina%20Cost (Default|GetSkillStats (Variables|Default|GetStats%20Component) (Variables|Default|GetSkill)))))
      (CallFunction|Done 3.0))))

(event EventActivateComboSkill
  (params (Hand :type E_Handed%20Enum :default "NewEnumerator0"))
  (bind _character (Variables|Default|GetCharacter))
  (bind _returnvalue (Transformation|GetActorLocation _character))
  ;[1 1 1] End through anim notify
  (if (CallFunction|IsGAActive)
    (bind (_outhit _returnvalue_2) (Collision|SphereTraceForObjects _returnvalue (+ _returnvalue (* (Transformation|GetActorForwardVector _character) 2e+02)) 4e+01 (Utilities|Array|MakeArray "ObjectTypeQuery9") false (Utilities|Array|MakeArray (Variables|Default|GetCharacter)) "ForDuration"))
    (if _returnvalue_2
      (bind _keys (Utilities|Map|Keys (Variables|/Game/DATA/Blueprints/Components/EquipmentComponet.EquipmentComponet_C|GetEquiped (Actor|GetComponentbyClass (.HitActor (Collision|BreakHitResult _outhit)) "/Game/DATA/Blueprints/Components/EquipmentComponet.EquipmentComponet_C"))))
      (bind _array_element (Utilities|Array|ForEachLoopwithBreak _keys)
        (:LoopBody
          (if (Utilities|Enum|Equal(Enum) (Variables|/Game/DATA/Blueprints/Actors/BP_MasterItem.BP_MasterItem_C|GetEquipType (.equipeditem (.Value (Utilities|Map|Find (Variables|/Game/DATA/Blueprints/Components/EquipmentComponet.EquipmentComponet_C|GetEquiped (Actor|GetComponentbyClass (.HitActor (Collision|BreakHitResult _outhit)) "/Game/DATA/Blueprints/Components/EquipmentComponet.EquipmentComponet_C")) _array_element)))) "NewEnumerator23")
            (Default|UnequipItem (Actor|GetComponentbyClass (.HitActor (Collision|BreakHitResult _outhit)) "/Game/DATA/Blueprints/Components/EquipmentComponet.EquipmentComponet_C") (.equipeditem (.Value (Utilities|Map|Find (Variables|/Game/DATA/Blueprints/Components/EquipmentComponet.EquipmentComponet_C|GetEquiped (Actor|GetComponentbyClass (.HitActor (Collision|BreakHitResult _outhit)) "/Game/DATA/Blueprints/Components/EquipmentComponet.EquipmentComponet_C")) _array_element))) (Utilities|GetClass (.equipeditem (.Value (Utilities|Map|Find (Variables|/Game/DATA/Blueprints/Components/EquipmentComponet.EquipmentComponet_C|GetEquiped (Actor|GetComponentbyClass (.HitActor (Collision|BreakHitResult _outhit)) "/Game/DATA/Blueprints/Components/EquipmentComponet.EquipmentComponet_C")) _array_element)))) true true)))
        (:Completed
          (CallFunction|Done 3.0)
          (Default|SetMeleeSkillUsed (Default|GetMainWeapon (Variables|/Game/DATA/BP_PC.BP_PC_C|GetCombatComponent (Variables|Default|GetCharacter))))
          (CallFunction|UnEquipHyperArmor))))))

(fn ConstructionScript
  (|CallParentFunction))