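; GA_RockThrow is an ability that makes the character throw a rock projectile along its aim.
; On GAStart, the CombatComponent runs an aim trace from the follow camera and the mesh's LHFS socket, giving the spawn transform for BP_ThrownRock.
; The rock receives range, speed, poise damage multiplier and friendly fire, then the RockThrow action is set on the CombatComponent.
; An unconnected alternative spawn aims at the player character with a slight pitch offset.
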(event EventBeginPlay
  (|CallParentFunction) ; This node is disabled and will not be called.\nDrag off pins to build functionality.
)

(event Collision|EventActorBeginOverlap
  (params (OtherActor :type Actor%20Object%20Reference)))

(event EventTick
  (params (DeltaSeconds :type Float%20%28single-precision%29)))

(event EventGAStart
  (bind _character (Variables|Default|GetCharacter))
  (bind _character_2 (Variables|Default|GetCharacter))
  (bind _returnvalue (Default|GetAimTrace (Variables|Default|GetCombat%20Component) (Variables|/Game/DATA/BP_PC.BP_PC_C|GetFollowCamera _character_2) (Variables|/Script/Engine.Character|GetMesh _character_2) 6e+03 2e+01 (Variables|/Game/DATA/Blueprints/Components/CombatComponent.CombatComponent_C|GetDraw%20Debug%20Type (Variables|Default|GetCombat%20Component)) true "LHFS" (Variables|Default|GetCharacter)))
  (Game|SpawnActorfromClass "/Game/DATA/Blueprints/Actors/Magic/BP_ThrownRock.BP_ThrownRock_C" _returnvalue "Undefined" "MultiplyWithRoot" _character 1.0 1e+01 6e+03 2e+03 _character 2.0 true _character)
  (Default|SetCurrentAction (Variables|Default|GetCombat%20Component) "(TagName=\"Character.Action.Skill/Magic.RockThrow\")"))

(fn ConstructionScript
  (|CallParentFunction))