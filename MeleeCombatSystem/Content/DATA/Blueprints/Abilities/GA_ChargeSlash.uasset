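; Charged Slash melee skill ability that extends the main weapon with a temporary growing blade.
; Start checks stamina, mana and combat state, draws the weapon if needed, then applies damage multiplier, hyper armor and the attack montage.
; ActivateComboSkill attaches the blade, redirects weapon collision to it and scales size, trail and trace radius by skill effectiveness.
; Ending restores collision and shrinks the blade, with Tick as fallback for overlapping blades.
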(event Custom|End
  (bind _default_collision_capsule_component (Variables|Default|GetDefault%20Collision%20Capsule%20Component))
  ;[1 1 1] Shrink&Delete
  (Variables|Default|SetActive false)
  (Default|SetCollisionMesh (Variables|/Game/DATA/Blueprints/Actors/BP_BaseWeapon.BP_BaseWeapon_C|GetMainWeaponCollisionComponent (Default|GetMainWeapon (Variables|/Game/DATA/BP_PC.BP_PC_C|GetCombatComponent (Variables|Default|GetCharacter)))) _default_collision_capsule_component _default_collision_capsule_component)
  (Variables|/Game/DATA/Blueprints/Components/CollosionComponent.CollosionComponent_C|SetTraceRadius (Variables|/Game/DATA/Blueprints/Actors/BP_BaseWeapon.BP_BaseWeapon_C|GetMainWeaponCollisionComponent (Default|GetMainWeapon (Variables|/Game/DATA/BP_PC.BP_PC_C|GetCombatComponent (Variables|Default|GetCharacter)))) (Variables|Default|GetDefault%20Trace%20Radius))
  (Utilities|IsValid (Variables|Default|GetBlade)
    (:Is%20Valid
      (bind _grow (Timeline|Timeline ReverseFromEnd)
        (:Update
          (Transformation|SetWorldScale3D (Variables|/Game/DATA/Blueprints/Actors/BP_BaseEquippable.BP_BaseEquippable_C|GetItemStaticMesh (Variables|Default|GetBlade)) (Math|Conversions|ToVector(Float) (Math|Float|Lerp 0.0 (* (.Effectiveness (Default|GetSkillStats (Variables|Default|GetStats%20Component) "(TagName=\"Character.Action.Skill/Magic.ChargedSlash\")")) 2.0) _grow)))
          (CallFunction|Done))
        (:Finished
          (Actor|DestroyActor (Variables|Default|GetBlade)))))))

(event Custom|Shrink
  ;[1 1 1] Shrink&Delete
  (bind _grow (Timeline|Timeline ReverseFromEnd)
    (:Update
      (Transformation|SetWorldScale3D (Variables|/Game/DATA/Blueprints/Actors/BP_BaseEquippable.BP_BaseEquippable_C|GetItemStaticMesh (Variables|Default|GetBlade)) (Math|Conversions|ToVector(Float) (Math|Float|Lerp 0.0 (* (.Effectiveness (Default|GetSkillStats (Variables|Default|GetStats%20Component) "(TagName=\"Character.Action.Skill/Magic.ChargedSlash\")")) 2.0) _grow)))
      (CallFunction|Done))
    (:Finished
      (Actor|DestroyActor (Variables|Default|GetBlade)))))

(event Custom|SwichedToOld
  ;[1 1 1] Shrink&Delete
  (bind _grow (Timeline|Timeline Stop)
    (:Update
      (Transformation|SetWorldScale3D (Variables|/Game/DATA/Blueprints/Actors/BP_BaseEquippable.BP_BaseEquippable_C|GetItemStaticMesh (Variables|Default|GetBlade)) (Math|Conversions|ToVector(Float) (Math|Float|Lerp 0.0 (* (.Effectiveness (Default|GetSkillStats (Variables|Default|GetStats%20Component) "(TagName=\"Character.Action.Skill/Magic.ChargedSlash\")")) 2.0) _grow)))
      (CallFunction|Done))
    (:Finished
      (Actor|DestroyActor (Variables|Default|GetBlade)))))

(event EventBeginPlay
  (|CallParentFunction) ; This node is disabled and will not be called.\nDrag off pins to build functionality.
)

(event Collision|EventActorBeginOverlap
  (params (OtherActor :type Actor%20Object%20Reference)))

(event EventGAStart
  (bind _stats_component (Variables|Default|GetStats%20Component))
  (bind _stats_component_2 (Variables|Default|GetStats%20Component))
  (bind _stats_component_3 (Variables|Default|GetStats%20Component))
  (bind (_mana_cost _stamina_cost) (Default|GetSkillStats _stats_component_3 "(TagName=\"Character.Action.Skill/Magic.ChargedSlash\")"))
  (bind (_mana_cost_2 _stamina_cost_2) (Default|GetSkillStats _stats_component_2 "(TagName=\"Character.Action.Skill/Magic.ChargedSlash\")"))
  ;[1 1 1] Start
  (if (not (Variables|Default|GetActive))
    (if (Math|Boolean|ANDBoolean (Default|StatGreaterThen _stats_component "NewEnumerator2" (Math|Conversions|ToFloat(Integer) _stamina_cost_2)) (Default|StatGreaterThen _stats_component "NewEnumerator4" (Math|Conversions|ToFloat(Integer) _mana_cost_2)) (Default|CanProformCombat (Variables|Default|GetCombat%20Component)))
      (Default|RotatetoTarget (Variables|Default|GetCharacter))
      (Utilities|IsCombatReady?
        (:Exit
          (bind _output_get (Variables|/Game/DATA/Blueprints/Actors/BP_BaseWeapon.BP_BaseWeapon_C|SetMeleSkillused (Default|GetMainWeapon (Variables|/Game/DATA/BP_PC.BP_PC_C|GetCombatComponent (Variables|Default|GetCharacter))) "(TagName=\"Character.Action.Skill/Magic.ChargedSlash\")"))
          (Default|SetActionDamageMultiplyer (Default|GetMainWeapon (Variables|/Game/DATA/BP_PC.BP_PC_C|GetCombatComponent (Variables|Default|GetCharacter))) _output_get (.Power (Default|GetSkillStats (Variables|Default|GetStats%20Component) "(TagName=\"Character.Action.Skill/Magic.ChargedSlash\")")) 1.5)
          (CallFunction|EquipHyperArmor)
          (Default|PerformComboAction (Variables|Default|GetCombat%20Component) false (Variables|Default|GetAttackMontages))
          (Default|SetState (Variables|Default|GetCombat%20Component) "(TagName=\"Character.State.GenralActionState\")")
          (Default|SetActionCost (Variables|Default|GetStats%20Component) "(TagName=\"Character.Action.Skill/Magic.ChargedSlash\")" (Math|Conversions|ToFloat(Integer) _stamina_cost) (Math|Conversions|ToFloat(Integer) _mana_cost))
          (Default|SetCurrentAction (Variables|Default|GetCombat%20Component) "(TagName=\"Character.Action.Skill/Magic.ChargedSlash\")")
          (CallFunction|Done)))
      (else
        (Default|OOMCheck (Variables|Default|GetStats%20Component) (Math|Conversions|ToFloat(Integer) (.Stamina%20Cost (Default|GetSkillStats (Variables|Default|GetStats%20Component) "(TagName=\"Character.Action.Skill/Magic.ChargedSlash\")"))))
        (CallFunction|Done)))))

(event EventActivateComboSkill
  (params (Hand :type E_Handed%20Enum :default "NewEnumerator0"))
  (bind _character (Variables|Default|GetCharacter))
  (bind _character_2 (Variables|Default|GetCharacter))
  (bind _stats_component (Variables|Default|GetStats%20Component))
  (bind _character_3 (Variables|Default|GetCharacter))
  (bind _character_4 (Variables|Default|GetCharacter))
  (bind _effectiveness (Default|GetSkillStats _stats_component "(TagName=\"Character.Action.Skill/Magic.ChargedSlash\")"))
  (bind _combatcomponent (Variables|/Game/DATA/BP_PC.BP_PC_C|GetCombatComponent _character_2))
  (bind _combatcomponent_2 (Variables|/Game/DATA/BP_PC.BP_PC_C|GetCombatComponent _character_3))
  (bind _combatcomponent_3 (Variables|/Game/DATA/BP_PC.BP_PC_C|GetCombatComponent _character_4))
  (bind _returnvalue (Default|GetMainWeapon _combatcomponent))
  (bind _returnvalue_2 (Default|GetMainWeapon _combatcomponent_2))
  (bind _returnvalue_3 (Default|GetMainWeapon _combatcomponent_3))
  (bind _itemstaticmesh (Variables|/Game/DATA/Blueprints/Actors/BP_BaseEquippable.BP_BaseEquippable_C|GetItemStaticMesh _returnvalue))
  (bind _mainweaponcollisioncomponent (Variables|/Game/DATA/Blueprints/Actors/BP_BaseWeapon.BP_BaseWeapon_C|GetMainWeaponCollisionComponent _returnvalue_2))
  (bind _mainweaponcollisioncomponent_2 (Variables|/Game/DATA/Blueprints/Actors/BP_BaseWeapon.BP_BaseWeapon_C|GetMainWeaponCollisionComponent _returnvalue_3))
  ;[1 1 1] Summon
  (if (not (Variables|Default|GetActive))
    (CallFunction|Done)
    (if (not (Utilities|IsValid (Variables|Default|GetBlade)))
      _
      (else
        (Variables|Default|SetBladeOld (Variables|Default|GetBlade))
        (Variables|Default|SetOldActive true)
        (CallFunction|SwichedtoOld)
        (CallFunction|StartTick)))
    (Variables|Default|SetActive true)
    (bind _returnvalue_4 (Game|SpawnActorfromClass "/Game/DATA/Blueprints/Actors/Useables/BP_ChargedSlashItem.BP_ChargedSlashItem_C" (Math|Transform|MakeTransform (+ (Transformation|GetSocketLocation _itemstaticmesh "WeaponStart") (* (Math|Vector|GetUpVector _itemstaticmesh) 3e+01)) (Transformation|GetWorldRotation _itemstaticmesh) "1.000000,1.000000,1.000000") "Undefined" "MultiplyWithRoot" _character "NewEnumerator1" 1 "NewEnumerator7" "NewEnumerator0" (Variables|/Game/DATA/BP_PC.BP_PC_C|GetInventory _character) 0 0 _character))
    (bind _output_get (Variables|Default|SetBlade _returnvalue_4))
    (Default|RemoveDropMesh _output_get)
    (Transformation|AttachActorToActor _output_get (Default|GetMainWeapon (Variables|/Game/DATA/BP_PC.BP_PC_C|GetCombatComponent (Variables|Default|GetCharacter))) "None" "KeepWorld" "KeepWorld" "KeepWorld" true)
    (Variables|Default|SetDefault%20Collision%20Capsule%20Component (Variables|/Game/DATA/Blueprints/Components/CollosionComponent.CollosionComponent_C|GetCollisionCapsuleComponent _mainweaponcollisioncomponent))
    (Variables|Default|SetDefault%20Trace%20Radius (Variables|/Game/DATA/Blueprints/Components/CollosionComponent.CollosionComponent_C|GetTraceRadius _mainweaponcollisioncomponent))
    (Default|SetCollisionMesh _mainweaponcollisioncomponent (Variables|/Game/DATA/Blueprints/Actors/BP_BaseEquippable.BP_BaseEquippable_C|GetItemStaticMesh (Variables|Default|GetBlade)) (Variables|/Game/DATA/Blueprints/Actors/BP_BaseEquippable.BP_BaseEquippable_C|GetItemStaticMesh (Variables|Default|GetBlade)))
    (Variables|/Game/DATA/Blueprints/Components/CollosionComponent.CollosionComponent_C|SetTraceRadius _mainweaponcollisioncomponent_2 (Math|Float|Clamp(Float) (* (* (Variables|/Game/DATA/Blueprints/Components/CollosionComponent.CollosionComponent_C|GetTraceRadius _mainweaponcollisioncomponent_2) 2.0) (.Effectiveness (Default|GetSkillStats (Variables|Default|GetStats%20Component) "(TagName=\"Character.Action.Skill/Magic.ChargedSlash\")"))) (* (* (Variables|/Game/DATA/Blueprints/Components/CollosionComponent.CollosionComponent_C|GetTraceRadius _mainweaponcollisioncomponent_2) 2.0) (.Effectiveness (Default|GetSkillStats (Variables|Default|GetStats%20Component) "(TagName=\"Character.Action.Skill/Magic.ChargedSlash\")"))) 75.0))
    (Utilities|IsValid (Variables|Default|GetBlade)
      (:Is%20Valid
        (bind _grow (Timeline|Grow PlayFromStart)
          (:Update
            (Transformation|SetWorldScale3D (Variables|/Game/DATA/Blueprints/Actors/BP_BaseEquippable.BP_BaseEquippable_C|GetItemStaticMesh (Variables|Default|GetBlade)) (Math|Vector|MakeVector (Math|Float|Clamp(Float) (Math|Float|Lerp 0.0 (* _effectiveness 2.0) _grow) (Math|Float|Lerp 0.0 (* _effectiveness 2.0) _grow) 5.0) (Math|Float|Clamp(Float) (Math|Float|Lerp 0.0 (* _effectiveness 2.0) _grow) (Math|Float|Lerp 0.0 (* _effectiveness 2.0) _grow) 5.0) (Math|Float|Lerp 0.0 (* _effectiveness 2.0) _grow)))
            (Niagara|SetNiagaraVariable(Float) (Variables|/Game/DATA/Blueprints/Actors/Useables/BP_ChargedSlashItem.BP_ChargedSlashItem_C|GetN_WeaponTrail (Variables|Default|GetBlade)) "Ribbon Width" (Math|Float|Lerp 0.0 (* _effectiveness 1e+02) _grow))
            (CallFunction|Done))))
      (:Is%20Not%20Valid
        (CallFunction|Done)))
    (else
      (CallFunction|End))))

(event EventDone
  (bind _default_collision_capsule_component (Variables|Default|GetDefault%20Collision%20Capsule%20Component))
  ;[1 1 1] Initiate end
  (|CallParentFunction)
  (Utilities|FlowControl|RetriggerableDelay 2.0)
  (CallFunction|UnEquipHyperArmor)
  (Variables|Default|SetActive false)
  (Default|SetCollisionMesh (Variables|/Game/DATA/Blueprints/Actors/BP_BaseWeapon.BP_BaseWeapon_C|GetMainWeaponCollisionComponent (Default|GetMainWeapon (Variables|/Game/DATA/BP_PC.BP_PC_C|GetCombatComponent (Variables|Default|GetCharacter)))) _default_collision_capsule_component _default_collision_capsule_component)
  (Variables|/Game/DATA/Blueprints/Components/CollosionComponent.CollosionComponent_C|SetTraceRadius (Variables|/Game/DATA/Blueprints/Actors/BP_BaseWeapon.BP_BaseWeapon_C|GetMainWeaponCollisionComponent (Default|GetMainWeapon (Variables|/Game/DATA/BP_PC.BP_PC_C|GetCombatComponent (Variables|Default|GetCharacter)))) (Variables|Default|GetDefault%20Trace%20Radius))
  (Variables|/Game/DATA/Blueprints/Actors/BP_BaseWeapon.BP_BaseWeapon_C|SetMeleSkillused (Default|GetMainWeapon (Variables|/Game/DATA/BP_PC.BP_PC_C|GetCombatComponent (Variables|Default|GetCharacter))) "")
  (Utilities|IsValid (Variables|Default|GetBlade)
    (:Is%20Valid
      (CallFunction|Shrink))))

(event EventTick
  (params (DeltaSeconds :type Float%20%28single-precision%29))
  (bind _returnvalue (Utilities|Time|GetWorldDeltaSeconds))
  (bind _bladeold (Variables|Default|GetBladeOld))
  (bind _itemstaticmesh (Variables|/Game/DATA/Blueprints/Actors/BP_BaseEquippable.BP_BaseEquippable_C|GetItemStaticMesh _bladeold))
  (bind _returnvalue_2 (Transformation|GetWorldScale _itemstaticmesh))
  (bind _returnvalue_3 (Math|Interpolation|FInterptoConstant (.x _returnvalue_2) 0.0 _returnvalue 1.0))
  ;[1 1 1] If anim speed is high this may activate to make sure both swords get deleted
  (if (Variables|Default|GetOldActive)
    (Transformation|SetWorldScale3D (Variables|/Game/DATA/Blueprints/Actors/BP_BaseEquippable.BP_BaseEquippable_C|GetItemStaticMesh (Variables|Default|GetBladeOld)) (Math|Conversions|ToVector(Float) _returnvalue_3))
    (if (== _returnvalue_3 0.0)
      (Actor|DestroyActor (Variables|Default|GetBladeOld))
      (Variables|Default|SetOldActive true)
      (CallFunction|StopTick))))

(fn ConstructionScript
  (|CallParentFunction))