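; Wind Pull ability: a held skill that spawns an attached BP_PullPickUps wind actor around the character, sized by the skill's Power and Effectiveness.
; Start requires the held key, combat readiness and a tenth of the skill's stamina and mana costs, then plays the cast montage.
; A recursive delay loop rechecks input and resources, awarding skill XP.
; Ending stops the wind, plays the end montage and clears nearby interaction prompts.
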(event Custom|End
  (bind _character (Variables|Default|GetCharacter))
  (bind _nearbyactorstointeract (Variables|/Game/DATA/BP_PC.BP_PC_C|GetNearByActorsToInteract _character))
  ;[1 1 1] End
  (Default|EndWind (Variables|Default|GetWind))
  (Animation|Montage|PlayMontage (Variables|/Script/Engine.Character|GetMesh (Variables|Default|GetCharacter)) (Variables|/Game/DATA/Blueprints/Components/CombatComponent.CombatComponent_C|GetWindPullAnimation (Variables|Default|GetCombat%20Component)) 1.0 0.0 "End"
    (:then
      (for _array_element _nearbyactorstointeract
        (Rendering|SetVisibility (.text _array_element) false false))
      (Utilities|Array|Clear _nearbyactorstointeract))))

(event Custom|HoldCheck
  (bind _stats_component (Variables|Default|GetStats%20Component))
  (bind _stats_component_2 (Variables|Default|GetStats%20Component))
  (bind (_mana_cost _stamina_cost) (Default|GetSkillStats _stats_component "(TagName=\"Character.Action.Skill/Magic.WindPull\")"))
  ;[1 1 1] Hold
  (if (CallFunction|Hold?)
    (Utilities|FlowControl|Delay 0.1)
    (CallFunction|Done 3.0)
    (if (and (Default|StatGreaterThen _stats_component_2 "NewEnumerator2" (* (Math|Conversions|ToFloat(Integer) _stamina_cost) 0.1)) (Default|StatGreaterThen _stats_component_2 "NewEnumerator4" (* (Math|Conversions|ToFloat(Integer) _mana_cost) 0.1)))
      (Default|SetCurrentAction (Variables|Default|GetCombat%20Component) "(TagName=\"Character.Action.Skill/Magic.WindPull\")")
      (Default|ModifySkillXP (Variables|Default|GetStats%20Component) "(TagName=\"Character.Action.Skill/Magic.WindPull\")" 1 true)
      (CallFunction|HoldCheck)
      (else
        (CallFunction|End)))
    (else
      (CallFunction|End))))

(event EventBeginPlay
  (|CallParentFunction) ; This node is disabled and will not be called.\nDrag off pins to build functionality.
)

(event Collision|EventActorBeginOverlap
  (params (OtherActor :type Actor%20Object%20Reference)))

(event EventTick
  (params (DeltaSeconds :type Float%20%28single-precision%29)))

(event EventActivateComboSkill
  (params (Hand :type E_Handed%20Enum :default "NewEnumerator0"))
  (bind _skill (Variables|Default|GetSkill))
  (bind _stats_component (Variables|Default|GetStats%20Component))
  (bind _stats_component_2 (Variables|Default|GetStats%20Component))
  (bind _skill_2 (Variables|Default|GetSkill))
  (bind _character (Variables|Default|GetCharacter))
  (bind (_mana_cost _stamina_cost) (Default|GetSkillStats _stats_component _skill_2))
  (bind (_mana_cost_2 _stamina_cost_2 _skill_xp _level_up_cost _skill_xpspent _skill_level _available_points _power _effectiveness) (Default|GetSkillStats _stats_component_2 _skill))
  ;[1 1 1] Spawn
  (if (CallFunction|IsGAActive)
    (CallFunction|FloatWeapon true "NewEnumerator2" "NewEnumerator5")
    (Default|SetActionCost _stats_component "(TagName=\"Character.Action.Skill/Magic.WindPull\")" (* (Math|Conversions|ToFloat(Integer) _stamina_cost) 0.1) (* (Math|Conversions|ToFloat(Integer) _mana_cost) 0.1))
    (CallFunction|Done 3.0)
    (Default|SetState (Variables|Default|GetCombat%20Component) "(TagName=\"Character.State.GenralActionState\")")
    (bind _returnvalue (Game|SpawnActorfromClass "/Game/DATA/Blueprints/Actors/Utility/BP_PullPickUps.BP_PullPickUps_C" (Transformation|GetActorTransform _character) "AlwaysSpawn" "MultiplyWithRoot" _character (* _power 1e+01) _effectiveness true _character))
    (Variables|Default|SetWind _returnvalue)
    (Transformation|AttachActorToActor _returnvalue _character "None" "SnapToTarget" "SnapToTarget" "KeepRelative" true)
    (CallFunction|HoldCheck)))

(event EventGAStart
  (bind _stats_component (Variables|Default|GetStats%20Component))
  (bind _stats_component_2 (Variables|Default|GetStats%20Component))
  (bind _skill (Variables|Default|GetSkill))
  (bind (_mana_cost _stamina_cost) (Default|GetSkillStats _stats_component_2 _skill))
  ;[1 1 1] Start
  (if (CallFunction|Hold?)
    (if (Math|Boolean|ANDBoolean (Default|StatGreaterThen _stats_component "NewEnumerator2" (* (Math|Conversions|ToFloat(Integer) _stamina_cost) 0.1)) (Default|StatGreaterThen _stats_component "NewEnumerator4" (* (Math|Conversions|ToFloat(Integer) _mana_cost) 0.1)) (Default|CanProformCombat (Variables|Default|GetCombat%20Component)))
      (Default|PerformComboAction (Variables|Default|GetCombat%20Component) false (Variables|Default|GetAttackMontages))
      (Default|SetState (Variables|Default|GetCombat%20Component) "(TagName=\"Character.State.GenralActionState\")")
      (else
        (Default|OOMCheck (Variables|Default|GetStats%20Component) (Math|Conversions|ToFloat(Integer) (.Stamina%20Cost (Default|GetSkillStats (Variables|Default|GetStats%20Component) (Variables|Default|GetSkill)))))
        (CallFunction|Done 3.0)))
    (else
      (CallFunction|Done 3.0))))

(fn ConstructionScript
  (|CallParentFunction))

(fn Hold?
  (return (and (Utilities|Enum|Equal(Enum) (.State (Default|GetKeyStates (Variables|Default|GetCharacter) (Variables|Default|GetKeyIndex))) "NewEnumerator1") (Default|GetCurrentStateNotEqualAny (Variables|Default|GetCombat%20Component) "(GameplayTags=((TagName=\"Character.Action.Skill/Magic.Jump\"),(TagName=\"Character.State.Dodging\"),(TagName=\"Character.Action.Stuned\"),(TagName=\"Character.State.Attacking\"),(TagName=\"Character.State.Dead\"),(TagName=\"Character.State.Disabled\")))"))))