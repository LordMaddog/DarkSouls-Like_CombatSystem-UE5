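; GA_FireStream is a gameplay ability actor for the fire stream magic skill.
; On start it checks stamina, mana and combat readiness, turns to target, plays a combo montage and enables hand effects and sound.
; ActivateComboSkill spawns BP_SpellFireStream ahead of the character, scaled by skill and sub stats, but charges RockThrow's costs.
; A retriggerable delay in Done then clears the effects and destroys the actor.
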(event EventBeginPlay
  (|CallParentFunction) ; This node is disabled and will not be called.\nDrag off pins to build functionality.
)

(event Collision|EventActorBeginOverlap
  (params (OtherActor :type Actor%20Object%20Reference)))

(event EventTick
  (params (DeltaSeconds :type Float%20%28single-precision%29)))

(event EventGAStart
  (bind _stats_component (Variables|Default|GetStats%20Component))
  (bind _stats_component_2 (Variables|Default|GetStats%20Component))
  (bind (_mana_cost _stamina_cost) (Default|GetSkillStats _stats_component_2 "(TagName=\"Character.Action.Skill/Magic.FireStream\")"))
  ;[1 1 1] Start
  (Utilities|FlowControl|Delay 0.2)
  (CallFunction|NPCGiveSkillifNoneExist "/Game/DATA/Blueprints/Actors/Useables/BP_FireStreamItem.BP_FireStreamItem_C" "(TagName=\"Character.Action.Skill/Magic.FireStream\")")
  (if (Math|Boolean|ANDBoolean (Default|StatGreaterThen _stats_component "NewEnumerator2" (Math|Conversions|ToFloat(Integer) _stamina_cost)) (Default|StatGreaterThen _stats_component "NewEnumerator4" (Math|Conversions|ToFloat(Integer) _mana_cost)) (Default|CanProformCombat (Variables|Default|GetCombat%20Component)))
    (Default|RotatetoTarget (Variables|Default|GetCharacter))
    (Default|PerformComboAction (Variables|Default|GetCombat%20Component) false (Variables|Default|GetAttackMontages))
    (Default|SetState (Variables|Default|GetCombat%20Component) "(TagName=\"Character.State.GenralActionState\")")
    (CallFunction|MagicHands "NewEnumerator2" "NewEnumerator2" true)
    (if (not (Utilities|IsValid (Variables|Default|GetSound)))
      (bind _returnvalue (Audio|SpawnSoundAttached "/Game/Migrated/Fire01_Cue.Fire01_Cue" (Variables|/Game/DATA/BP_PC.BP_PC_C|GetVoice (Variables|Default|GetCharacter)) "None" "0, 0, 0" "0, 0, 0" "KeepRelativeOffset" false 1.0 1.0 0.0 0 0))
      (Variables|Default|SetSound _returnvalue)
      (Utilities|FlowControl|Delay 0.2)
      (Audio|Components|Audio|FadeOut _returnvalue 2.0 0.0 "Linear" :!class /Script/Engine.AudioComponent)
      (else
        (Audio|Components|Audio|FadeOut (Variables|Default|GetSound) 2.0 0.0 "Linear" :!class /Script/Engine.AudioComponent)))
    (else
      (Default|OOMCheck (Variables|Default|GetStats%20Component) (Math|Conversions|ToFloat(Integer) (.Stamina%20Cost (Default|GetSkillStats (Variables|Default|GetStats%20Component) "(TagName=\"Character.Action.Skill/Magic.FireStream\")"))))
      (CallFunction|Done 3.0))))

(event EventActivateComboSkill
  (params (Hand :type E_Handed%20Enum :default "NewEnumerator0"))
  (bind _character (Variables|Default|GetCharacter))
  (bind _character_2 (Variables|Default|GetCharacter))
  (bind _stats_component (Variables|Default|GetStats%20Component))
  (bind _stats_component_2 (Variables|Default|GetStats%20Component))
  (bind (_mana_cost _stamina_cost _skill_xp _level_up_cost _skill_level _available_points _power _effectiveness) (Default|GetSkillStats _stats_component "(TagName=\"Character.Action.Skill/Magic.FireStream\")"))
  (bind (_mana_cost_2 _stamina_cost_2) (Default|GetSkillStats _stats_component_2 "(TagName=\"Character.Action.Skill/Magic.RockThrow\")"))
  (bind _value (Default|GetSubStats _stats_component "NewEnumerator12"))
  (bind _returnvalue (* _value _power))
  (bind _returnvalue_2 (* _returnvalue 0.1))
  (bind _returnvalue_3 (+ _effectiveness _returnvalue_2))
  ;[1 1 1] Spawn
  (CallFunction|Done 3.0)
  (Default|SetActionCost (Variables|Default|GetStats%20Component) "(TagName=\"Character.Action.Skill/Magic.FireStream\")" (Math|Conversions|ToFloat(Integer) _stamina_cost_2) (Math|Conversions|ToFloat(Integer) _mana_cost_2))
  (Default|SetCurrentAction (Variables|Default|GetCombat%20Component) "(TagName=\"Character.Action.Skill/Magic.FireStream\")")
  (Game|SpawnActorfromClass "/Game/DATA/Blueprints/Actors/BP_SpellFireStream.BP_SpellFireStream_C" (Math|Transform|MakeTransform (+ (+ (Transformation|GetActorLocation _character_2) (* (Transformation|GetActorForwardVector _character_2) 5e+01)) "0.000000,0.000000,40.000000") (Math|Rotator|MakeRotator 0.0 0.0 (.yaw (Transformation|GetActorRotation _character_2))) (Math|Conversions|ToVector(Float) _returnvalue_3)) "Undefined" "MultiplyWithRoot" _character _returnvalue_3 _power 0.0 6e+03 0.0 _character _effectiveness true "(TagName=\"Character.Action.Skill/Magic.FireStream\")" false 0.0 _character))

(event EventDone
  (params (Duration :type Float%20%28single-precision%29))
  (bind _sound (Variables|Default|GetSound))
  ;[1 1 1] End
  (Utilities|FlowControl|RetriggerableDelay Duration)
  (CallFunction|MagicHands "NewEnumerator2" "NewEnumerator2" false)
  (if (not (Utilities|IsValid _sound))
    _
    (else
      (Audio|Components|Audio|FadeOut _sound 2.0 0.0 "Linear" :!class /Script/Engine.AudioComponent)))
  (Actor|DestroyActor))

(fn ConstructionScript
  (|CallParentFunction))