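; Power Slash ability actor that spawns a BP_PowerSlice in front of the character when the ability starts.
; GAStart places the slice ahead of the mesh's RHFS socket, aligned to the character's forward vector, with the character as owner and instigator.
; It configures the slice with area, range, zero initial speed and a boosted poise damage multiplier, then destroys itself after a brief delay.
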(event EventBeginPlay
  (|CallParentFunction) ; This node is disabled and will not be called.\nDrag off pins to build functionality.
)

(event Collision|EventActorBeginOverlap
  (params (OtherActor :type Actor%20Object%20Reference)))

(event EventTick
  (params (DeltaSeconds :type Float%20%28single-precision%29)))

(event EventGAStart
  (bind _character (Variables|Default|GetCharacter))
  (bind _character_2 (Variables|Default|GetCharacter))
  (bind _returnvalue (Transformation|GetActorForwardVector _character))
  (Game|SpawnActorfromClass "/Game/DATA/Blueprints/Actors/Magic/BP_PowerSlice.BP_PowerSlice_C" (Math|Transform|MakeTransform (+ (* _returnvalue 1e+02) (Transformation|GetSocketLocation (Variables|/Script/Engine.Character|GetMesh _character) "RHFS")) (Math|Conversions|RotationFromXVector _returnvalue) "1.000000,1.000000,1.000000") "AlwaysSpawn" "MultiplyWithRoot" _character_2 1.0 1.2e+02 2e+02 0.0 _character_2 2.0 false _character_2)
  (Utilities|FlowControl|Delay 0.2)
  (Actor|DestroyActor))

(fn ConstructionScript
  (|CallParentFunction))