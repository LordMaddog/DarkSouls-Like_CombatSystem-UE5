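; Channeled crafting ability actor that feeds the skill's Power into a BuildItem while the character holds still.
; GAStart checks stamina and mana, then plays a motion-warped montage; ActivateComboSkill starts a one-second loop granting skill XP.
; Movement, low resources or forced end zeroes craft power and plays the exit montage; a retriggerable delay destroys the actor once refreshes stop.
; GetNewBuildItem can find nearby unfinished builds but is not called here; disconnected rock-throw nodes remain.
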(event Custom|Continue
  (bind (_returnvalue _returnvalue1) (CallFunction|EnoughManaorStamina))
  ;[1 1 1] Channel
  (if (and (Class|KismetMathLibrary|NearlyEqualTransformTransform (Variables|Default|GetActorTransform) (Transformation|GetActorTransform (Variables|Default|GetCharacter)) 1e+01 1e+01 1e+01) (Variables|Default|GetActive))
    (if _returnvalue
      (Default|ModifySkillXP (Variables|Default|GetStats%20Component) (Variables|Default|GetSkill) 1 true)
      (CallFunction|Done 3.0)
      (Default|SetCurrentAction (Variables|Default|GetCombat%20Component) (Variables|Default|GetSkill))
      (Utilities|FlowControl|Delay 1.0)
      (CallFunction|Continue)
      (else
        (Default|OOMCheck (Variables|Default|GetStats%20Component) _returnvalue1)
        (CallFunction|Stop :!label _label)))
    (else
      (goto _label))))

(event Custom|Stop
  ;[1 1 1] Stop
  (Utilities|FlowControl|DoOnce false
    (:Completed
      (Default|PerformComboAction (Variables|Default|GetCombat%20Component) false (Variables|Default|GetAttackMontagesTwo))
      (Class|BuildBPI|CraftPower(Message) (Variables|Default|GetBuildItem) 0.0)
      (Variables|Default|SetActive false))))

(event Custom|Reset
  ;[1 1 1] Stop
  (Utilities|FlowControl|DoOnce false) ; enters at Reset
)

(event EventBeginPlay
  (|CallParentFunction) ; This node is disabled and will not be called.\nDrag off pins to build functionality.
)

(event Collision|EventActorBeginOverlap
  (params (OtherActor :type Actor%20Object%20Reference)))

(event EventTick
  (params (DeltaSeconds :type Float%20%28single-precision%29)))

(event EventGAStart
  (bind (_returnvalue _returnvalue1) (CallFunction|EnoughManaorStamina))
  ;[1 1 1] Start
  (if _returnvalue
    (Default|RotatetoTarget (Variables|Default|GetCharacter))
    (CallFunction|Done 3.0)
    (Class|CombatBPI|UpdateMotionWarp(Message) (Variables|Default|GetCharacter) "Crafting" (Variables|Default|GetWarpTarget))
    (Default|PerformComboAction (Variables|Default|GetCombat%20Component) false (Variables|Default|GetAttackMontages))
    (Default|SetState (Variables|Default|GetCombat%20Component) "(TagName=\"Character.State.GenralActionState\")")
    (CallFunction|MagicHands "NewEnumerator2" "NewEnumerator3" true)
    (else
      (Default|OOMCheck (Variables|Default|GetStats%20Component) _returnvalue1)
      (CallFunction|Done 3.0))))

(event EventActivateComboSkill
  (params (Hand :type E_Handed%20Enum :default "NewEnumerator0"))
  (bind _stats_component (Variables|Default|GetStats%20Component))
  (bind _skill (Variables|Default|GetSkill))
  (bind (_mana_cost _stamina_cost) (Default|GetSkillStats _stats_component _skill))
  ;[1 1 1] Spawn
  (if (CallFunction|IsGAActive)
    (Variables|Default|SetActive true)
    (CallFunction|Done 3.0)
    (Default|SetActionCost _stats_component (Variables|Default|GetSkill) (Math|Conversions|ToFloat(Integer) _stamina_cost) (Math|Conversions|ToFloat(Integer) _mana_cost))
    (Default|SetCurrentAction (Variables|Default|GetCombat%20Component) (Variables|Default|GetSkill))
    (Class|BuildBPI|CraftPower(Message) (Variables|Default|GetBuildItem) (.Power (Default|GetSkillStats (Variables|Default|GetStats%20Component) (Variables|Default|GetSkill))))
    (CallFunction|Reset)
    (Utilities|FlowControl|Delay 1.0)
    (Variables|Default|SetActorTransform (Transformation|GetActorTransform (Variables|Default|GetCharacter)))
    (CallFunction|Continue)))

(event EventDone
  (params (Duration :type Float%20%28single-precision%29))
  ;[1 1 1] End
  (Utilities|FlowControl|RetriggerableDelay Duration)
  (CallFunction|MagicHands "NewEnumerator2" "NewEnumerator3" false)
  (Default|RemoveGA (Variables|/Game/DATA/BP_PC.BP_PC_C|GetCombatComponent (Variables|Default|GetCharacter)) (Utilities|GetClass self))
  (Actor|DestroyActor))

(event EventGAForceEnd
  ;[1 1 1] Channel
  (CallFunction|Stop))

(fn ConstructionScript
  (|CallParentFunction))

(fn GetNewBuildItem
  (bind _actortransform (Variables|Default|GetActorTransform))
  (bind (_outhits _returnvalue) (Collision|MultiSphereTraceForObjects (.location _actortransform) (.location _actortransform) (* (.Power (Default|GetSkillStats (Variables|Default|GetStats%20Component) (Variables|Default|GetSkill))) 1e+02) (Utilities|Array|MakeArray "ObjectTypeQuery7") false (Utilities|Array|MakeArray (Variables|Default|GetCharacter)) "None"))
  (for _array_element _outhits
    (if _returnvalue
      (bind _builditem (Class|BuildBPI|GetBuildItem(Message) (.hitactor _array_element)))
      (Utilities|IsValid _builditem
        (:Is%20Valid
          (if (not (Variables|/Game/DATA/Blueprints/Actors/BuildItems/BP_MasterBuild.BP_MasterBuild_C|GetIsBuildDone _builditem))
            (Variables|Default|SetBuildItem _builditem)
            (Variables|/Game/DATA/Blueprints/Actors/BuildItems/BP_MasterBuild.BP_MasterBuild_C|SetPlayer _builditem (Variables|Default|GetCharacter))
            (return true))))))
  (return false))

(fn EnoughManaorStamina
  (bind _stats_component (Variables|Default|GetStats%20Component))
  (bind _stats_component_2 (Variables|Default|GetStats%20Component))
  (bind _skill (Variables|Default|GetSkill))
  (bind (_mana_cost _stamina_cost) (Default|GetSkillStats _stats_component_2 _skill))
  (bind _returnvalue (Math|Conversions|ToFloat(Integer) _stamina_cost))
  (return (and (Default|StatGreaterThen _stats_component "NewEnumerator2" _returnvalue) (Default|StatGreaterThen _stats_component "NewEnumerator4" (Math|Conversions|ToFloat(Integer) _mana_cost))) _returnvalue))