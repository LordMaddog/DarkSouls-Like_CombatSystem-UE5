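; Ability actor for the Icy Earth Smash skill, which spawns a BP_EarthSmash on the ground in front of the character.
; If two stat checks pass, it plays the smash montage at a stat-driven rate and sets combat state and action; otherwise it calls OOMCheck.
; The montage notify traces downward ahead of the character and spawns the smash at the hit point.
; The ability destroys itself shortly after blend-out.
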(event EventBeginPlay
  (|CallParentFunction) ; This node is disabled and will not be called.\nDrag off pins to build functionality.
)

(event Collision|EventActorBeginOverlap
  (params (OtherActor :type Actor%20Object%20Reference)))

(event EventTick
  (params (DeltaSeconds :type Float%20%28single-precision%29)))

(event EventEarthSmash
  (CallFunction|StartAbility))

(event EventStartAbility
  (bind _character (Variables|Default|GetCharacter))
  (bind _stats_component (Variables|Default|GetStats%20Component))
  (bind _character_2 (Variables|Default|GetCharacter))
  (bind _character_3 (Variables|Default|GetCharacter))
  (bind _returnvalue (Transformation|GetActorForwardVector _character_3))
  (bind _returnvalue_2 (Transformation|GetActorLocation _character_3))
  (bind _returnvalue_3 (* _returnvalue 1e+02))
  (bind _returnvalue_4 (+ _returnvalue_2 _returnvalue_3))
  (if (and (Default|StatGreaterThen _stats_component "NewEnumerator2" 3.0) (Default|StatGreaterThen _stats_component "NewEnumerator4" 3.0))
    (Animation|Montage|PlayMontage (Variables|/Script/Engine.Character|GetMesh (Variables|Default|GetCharacter)) (Variables|/Game/DATA/Blueprints/Components/CombatComponent.CombatComponent_C|GetEarthSmashAnimation (Variables|Default|GetCombat%20Component)) (Default|GetSubStats (Variables|Default|GetStats%20Component) "NewEnumerator19")
      (:then
        (Default|SetState (Variables|Default|GetCombat%20Component) "(TagName=\"Character.State.GenralActionState\")")
        (Default|SetCurrentAction (Variables|Default|GetCombat%20Component) "(TagName=\"Character.Action.Skill/Magic.EarthSmash\")"))
      (:OnBlendOut
        (Utilities|FlowControl|Delay 3.0)
        (Actor|DestroyActor))
      (:OnNotifyBegin
        (bind (_outhit _returnvalue_5) (Collision|LineTraceByChannel _returnvalue_4 (- _returnvalue_4 "0.000000,0.000000,150.000000") "TraceTypeQuery1" false (Utilities|Array|MakeArray _character_2) (Variables|/Game/DATA/Blueprints/Components/CombatComponent.CombatComponent_C|GetDraw%20Debug%20Type (Variables|/Game/DATA/BP_PC.BP_PC_C|GetCombatComponent _character_2))))
        (if _returnvalue_5
          (Game|SpawnActorfromClass "/Game/DATA/Blueprints/Actors/Magic/BP_EarthSmash.BP_EarthSmash_C" (Math|Transform|MakeTransform (+ (.Location (Collision|BreakHitResult _outhit)) "0.000000,0.000000,10.000000") (Transformation|GetActorRotation (Variables|Default|GetCharacter)) "1.500000,1.500000,1.500000") "AlwaysSpawn" "MultiplyWithRoot" _character 1.0 157.441377 1.5e+02 0.0 _character 1.5 false _character))))
    (else
      (Default|OOMCheck (Variables|Default|GetStats%20Component) 3.0))))

(event EventGAStart
  (CallFunction|StartAbility))

(fn ConstructionScript
  (|CallParentFunction))