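; GA_GiantSmash is an ability actor that spawns an earth smash effect on the ground beneath the character's weapon.
; GAStart and EarthSmash both run StartAbility, which traces downward from an offset beside the WeaponSocket.
; On a hit it spawns a scaled, stationary BP_EarthSmash, pulled back along the character's forward axis, with a heavy impact sound.
; It then sets the combat component's current action to EarthSmash.
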(event EventBeginPlay
  (|CallParentFunction) ; This node is disabled and will not be called.\nDrag off pins to build functionality.
)

(event Collision|EventActorBeginOverlap
  (params (OtherActor :type Actor%20Object%20Reference)))

(event EventTick
  (params (DeltaSeconds :type Float%20%28single-precision%29)))

(event EventEarthSmash
  (CallFunction|StartAbility))

(event EventStartAbility
  (bind _character (Variables|Default|GetCharacter))
  (bind _character_2 (Variables|Default|GetCharacter))
  (bind _character_3 (Variables|Default|GetCharacter))
  (bind _returnvalue (Transformation|GetActorRightVector _character_3))
  (bind _mesh (Variables|/Script/Engine.Character|GetMesh _character_3))
  (bind _returnvalue_2 (Transformation|GetSocketLocation _mesh "WeaponSocket"))
  (bind _returnvalue_3 (* _returnvalue -5e+01))
  (bind _returnvalue_4 (+ _returnvalue_2 _returnvalue_3))
  (bind (_outhit _returnvalue_5) (Collision|LineTraceByChannel _returnvalue_4 (- _returnvalue_4 "0.000000,0.000000,150.000000") "TraceTypeQuery1" false (Utilities|Array|MakeArray _character_2) (Variables|/Game/DATA/Blueprints/Components/CombatComponent.CombatComponent_C|GetDraw%20Debug%20Type (Variables|/Game/DATA/BP_PC.BP_PC_C|GetCombatComponent _character_2))))
  (if _returnvalue_5
    (bind _returnvalue_6 (Game|SpawnActorfromClass "/Game/DATA/Blueprints/Actors/Magic/BP_EarthSmash.BP_EarthSmash_C" (Math|Transform|MakeTransform (+ (.Location (Collision|BreakHitResult _outhit)) (* (Transformation|GetActorForwardVector (Variables|Default|GetCharacter)) -2.5e+02)) (Transformation|GetActorRotation (Variables|Default|GetCharacter)) "2.500000,2.500000,1.500000") "AlwaysSpawn" "MultiplyWithRoot" _character 1.0 257.441377 1.5e+02 0.0 _character 1.0 false _character))
    (Audio|Components|Audio|SetSound (Variables|/Game/DATA/Blueprints/Actors/BP_BaseSpell.BP_BaseSpell_C|GetExplosiveSound _returnvalue_6) "/Game/DATA/AI/FrostGiantBoss/Sounds/SC_HeavyImpact.SC_HeavyImpact")
    (Default|SetCurrentAction (Variables|Default|GetCombat%20Component) "(TagName=\"Character.Action.Skill/Magic.EarthSmash\")")))

(event EventGAStart
  (CallFunction|StartAbility))

(fn ConstructionScript
  (|CallParentFunction))