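; Bow-and-arrow ability actor that lets players and NPCs draw, hold and fire equipped arrows.
; GAStart checks resources, arrows and drawn weapon, then plays pull montages; ActivateComboSkill attaches an arrow to the hand, timer-aligned until key release or a random NPC hold ends.
; Launch plays release montages; an anim-notify Fired event aims by trace, scales damage and speed by charge ticks, sets gravity from arrow weight and consumes player ammo.
; A retriggerable Done delay cleans up the ability.
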(event Custom|ContinueCharge
  (bind _character (Variables|Default|GetCharacter))
  (bind _mesh (Variables|/Script/Engine.Character|GetMesh _character))
  (bind _returnvalue (Transformation|GetSocketLocation _mesh "RHFS"))
  (bind _returnvalue_2 (Transformation|GetSocketLocation _mesh "LHFS"))
  (bind _returnvalue_3 (+ _returnvalue_2 "0.000000,0.000000,8.000000"))
  (bind _returnvalue_4 (Math|Rotator|FindLookatRotation _returnvalue _returnvalue_3))
  ;[1 1 1] Contuinue
  (Utilities|IsValid (Variables|Default|GetCharacter)
    (:Is%20Valid
      (if (select (Variables|/Game/DATA/Blueprints/Components/CombatComponent.CombatComponent_C|GetIsPlayer (Variables|Default|GetCombat%20Component)) (Utilities|Enum|Equal(Enum) (.State (Default|GetKeyStates (Variables|Default|GetCharacter) (Variables|Default|GetKeyIndex))) "NewEnumerator1") (Variables|Default|GetHold))
        (CallFunction|Done 3.0)
        (Transformation|SetWorldRotation (Variables|/Game/DATA/Blueprints/Actors/BP_BaseSpell.BP_BaseSpell_C|GetMainProjectileCore (Variables|Default|GetArrow)) (Math|Rotator|MakeRotator (.roll _returnvalue_4) (.pitch _returnvalue_4) (+ (.yaw _returnvalue_4) -2.0)) false false)
        (else
          (CallFunction|Launch))))
    (:Is%20Not%20Valid
      (Actor|DestroyActor))))

(event Custom|Launch
  ;[1 1 1] Launch
  (if (Variables|Default|GetCharging)
    (Variables|Default|SetCharging false)
    (Default|PerformComboAction (Variables|Default|GetCombat%20Component) false (Variables|Default|GetAttackMontages2))
    (Animation|Montage|MontagePlay (Components|SkeletalMesh|GetAnimInstance (.ItemSkeletalMesh (CallFunction|GetBow))) "/Game/DATA/Animations/Bow/BowSkelAnimations/Default_Montage.Default_Montage" 1.0 "MontageLength" 0.0 true)))

(event Custom|fired
  (bind _tick_count (Variables|Default|GetTick%20Count))
  (bind _returnvalue (* _tick_count 0.1))
  (bind _returnvalue_2 (* _returnvalue 4e+04))
  ;[1 1 1] Shoots off Arrow. (is called by anim notify)
  (Utilities|IsValid (Variables|Default|GetArrow)
    (:Is%20Valid
      (Transformation|DetachFromActor (Variables|Default|GetArrow) "KeepWorld" "KeepWorld" "KeepWorld")
      (Components|Activation|Activate (Variables|/Game/DATA/Blueprints/Actors/BP_BaseSpell.BP_BaseSpell_C|GetProjectileMovement (Variables|Default|GetArrow)) true)
      (Utilities|Time|ClearandInvalidateTimerbyHandle (Variables|Default|GetTimer))
      (Variables|/Game/DATA/Blueprints/Actors/BP_BaseSpell.BP_BaseSpell_C|SetDamageMultiplier (Variables|Default|GetArrow) (- (+ (* (* (Variables|Default|GetTick%20Count) 0.1) 1.5) (Variables|/Game/DATA/Blueprints/Actors/BP_BaseWeapon.BP_BaseWeapon_C|GetWeaponMultiplierDamage (Default|GetMainWeapon (Variables|Default|GetCombat%20Component)))) 1.0))
      (Default|DamageCalculate (Variables|Default|GetArrow))
      (CallFunction|PlayBowSwingandArrowSound)
      (bind _returnvalue_3 (Default|GetAimTrace (Variables|Default|GetCombat%20Component) (Variables|/Game/DATA/BP_PC.BP_PC_C|GetFollowCamera (Variables|Default|GetCharacter)) (Variables|/Game/DATA/Blueprints/Actors/BP_BaseSpell.BP_BaseSpell_C|GetVisualEffect (Variables|Default|GetArrow)) 6e+03 2e+01 (Variables|/Game/DATA/Blueprints/Components/CombatComponent.CombatComponent_C|GetDraw%20Debug%20Type (Variables|Default|GetCombat%20Component)) false "LHFS" (Variables|Default|GetArrow)))
      (Transformation|SetActorRotation (Variables|Default|GetArrow) (select (Variables|/Game/DATA/Blueprints/Components/CombatComponent.CombatComponent_C|GetIsPlayer (Variables|Default|GetCombat%20Component)) (.rotation _returnvalue_3) (Math|Rotator|MakeRotator (.Roll (Math|Rotator|BreakRotator (.rotation _returnvalue_3))) (+ (.Pitch (Math|Rotator|BreakRotator (.rotation _returnvalue_3))) 1.5) (.Yaw (Math|Rotator|BreakRotator (.rotation _returnvalue_3))))))
      (Game|Components|ProjectileMovement|SetVelocityinLocalSpace (Variables|/Game/DATA/Blueprints/Actors/BP_BaseSpell.BP_BaseSpell_C|GetProjectileMovement (Variables|Default|GetArrow)) (Math|Vector|MakeVector (Math|Float|Clamp(Float) _returnvalue_2 5e+02 _returnvalue_2) 0.0 0.0))
      (Variables|/Script/Engine.ProjectileMovementComponent|SetProjectileGravityScale (Variables|/Game/DATA/Blueprints/Actors/BP_BaseSpell.BP_BaseSpell_C|GetProjectileMovement (Variables|Default|GetArrow)) (CallFunction|GetArrowsWeight))
      (CallFunction|Done 1.0)
      (CallFunction|Reset)
      (Collision|SetCollisionEnabled (Variables|/Game/DATA/Blueprints/Actors/BP_BaseSpell.BP_BaseSpell_C|GetMainProjectileCore (Variables|Default|GetArrow)) "QueryAndPhysics")
      (Variables|Default|SetArrow 0)
      (CallFunction|RemoveArrow)
      (Class|AnimBPI|BowAiming(Message) (Components|SkeletalMesh|GetAnimInstance (Variables|/Script/Engine.Character|GetMesh (Variables|Default|GetCharacter))) false)
      (Actor|Tick|SetActorTickEnabled false)
      (Audio|Components|Audio|Stop (Variables|Default|GetDraw%20Bow%20Sound)))
    (:Is%20Not%20Valid
      ;[1 1 1] End GA
      (Utilities|IsValid (Variables|Default|GetCharacter)
        (:Is%20Valid
          (CallFunction|FloatWeapon false "NewEnumerator2" "NewEnumerator2")
          (Default|RemoveGA (Variables|/Game/DATA/BP_PC.BP_PC_C|GetCombatComponent (Variables|Default|GetCharacter)) (Utilities|GetClass self))
          (Default|SetState (Variables|Default|GetCombat%20Component))
          (Actor|DestroyActor))))))

(event Custom|Reset
  (bind (_value _equipedarrows) (CallFunction|IsThereAnyArrows))
  (bind _character (Variables|Default|GetCharacter))
  (bind _skill (Variables|Default|GetSkill))
  (bind (_stamina _mana) (CallFunction|CheckManaStamina _skill))
  (bind _combatcomponent (Variables|/Game/DATA/BP_PC.BP_PC_C|GetCombatComponent _character))
  ;[1 1 1] Start
  (Utilities|FlowControl|DoOnce false) ; enters at Reset
)

(event EventBeginPlay
  (|CallParentFunction) ; This node is disabled and will not be called.\nDrag off pins to build functionality.
)

(event Collision|EventActorBeginOverlap
  (params (OtherActor :type Actor%20Object%20Reference)))

(event EventGAStart
  (bind (_value _equipedarrows) (CallFunction|IsThereAnyArrows))
  (bind _character (Variables|Default|GetCharacter))
  (bind _skill (Variables|Default|GetSkill))
  (bind (_stamina _mana) (CallFunction|CheckManaStamina _skill))
  (bind _combatcomponent (Variables|/Game/DATA/BP_PC.BP_PC_C|GetCombatComponent _character))
  ;[1 1 1] Start
  (if (Variables|/Game/DATA/Blueprints/Components/CombatComponent.CombatComponent_C|GetIsPlayer (Variables|Default|GetCombat%20Component))
    _
    (else
      (Utilities|FlowControl|Delay 0.1)
      (CallFunction|NPCGiveSkillifNoneExist "/Game/DATA/Blueprints/Actors/Useables/BP_ArcherySkillItem.BP_ArcherySkillItem_C" (Variables|Default|GetSkill))))
  (Utilities|FlowControl|DoOnce false
    (:Completed
      (if (Math|Boolean|ANDBoolean _stamina _mana (Default|CanProformCombat (Variables|Default|GetCombat%20Component)))
        (Default|RotatetoTarget (Variables|Default|GetCharacter))
        (if (Default|GetCombatEnabled _combatcomponent)
          (if _value
            (Variables|Default|SetEquiped%20Arrows _equipedarrows)
            (Default|RotatetoTarget (Variables|Default|GetCharacter))
            (CallFunction|PullAnimation (select (Variables|/Game/DATA/Blueprints/Components/CombatComponent.CombatComponent_C|GetIsPlayer (Variables|Default|GetCombat%20Component)) (+ (.Power (Default|GetSkillStats (Variables|Default|GetStats%20Component) (Variables|Default|GetSkill))) 0.5) 2.0))
            (Default|SetState (Variables|Default|GetCombat%20Component) "(TagName=\"Character.State.GenralActionState\")")
            (Variables|Default|SetCharging true)
            (Variables|Default|SetDrawling true)
            (CallFunction|Done 5.0)
            (Variables|Default|SetTick%20Count 0.0)
            (Variables|Default|SetHold true)
            (Class|AnimBPI|BowAiming(Message) (Components|SkeletalMesh|GetAnimInstance (Variables|/Script/Engine.Character|GetMesh (Variables|Default|GetCharacter))) true)
            (else
              (CallFunction|Done 3.0 :!label _label)
              (CallFunction|Reset)))
          (else
            (Default|Draw/sheathWeapon _combatcomponent)
            (goto _label)))
        (else
          (Default|OOMCheck (Variables|Default|GetStats%20Component) (Math|Conversions|ToFloat(Integer) (.Stamina%20Cost (Default|GetSkillStats (Variables|Default|GetStats%20Component) (Variables|Default|GetSkill)))))
          (CallFunction|Done 5.0)
          (CallFunction|Reset))))))

(event EventActivateComboSkill
  (params (Hand :type E_Handed%20Enum :default "NewEnumerator0"))
  (bind _character (Variables|Default|GetCharacter))
  (bind _character_2 (Variables|Default|GetCharacter))
  ;[1 1 1] Spawn
  (if (Variables|Default|GetCharging)
    (CallFunction|SetCost)
    (CallFunction|Done 5.0)
    (Default|SetState (Variables|Default|GetCombat%20Component) "(TagName=\"Character.State.GenralActionState\")")
    (bind _returnvalue (Default|GetAimTrace (Variables|Default|GetCombat%20Component) (Variables|/Game/DATA/BP_PC.BP_PC_C|GetFollowCamera _character_2) (Variables|/Script/Engine.Character|GetMesh _character_2) 6e+03 2e+01 (Variables|/Game/DATA/Blueprints/Components/CombatComponent.CombatComponent_C|GetDraw%20Debug%20Type (Variables|Default|GetCombat%20Component)) true "RHFS" (Variables|Default|GetCharacter)))
    (bind _returnvalue_2 (Game|SpawnActorfromClass "/Game/DATA/Blueprints/Actors/Magic/BP_BaseArrowSpell.BP_BaseArrowSpell_C" (Math|Transform|MakeTransform (+ (Transformation|GetSocketLocation (Variables|/Script/Engine.Character|GetMesh (Variables|Default|GetCharacter)) "RHFS") "0.000000,0.000000,2.000000") (.rotation _returnvalue) "1.000000,1.000000,1.000000") "Undefined" "MultiplyWithRoot" _character 1.0 1e+01 2e+04 0.0 _character (- (+ (Variables|/Game/DATA/Blueprints/Actors/BP_BaseWeapon.BP_BaseWeapon_C|GetBasePoiseDamgeMultiplier (Default|GetMainWeapon (Variables|Default|GetCombat%20Component))) (.Effectiveness (Default|GetSkillStats (Variables|Default|GetStats%20Component) (Variables|Default|GetSkill)))) 1.0) true "(TagName=\"Character.Action.Skill/Magic.Archery\")" false 0.0 _character))
    (bind _output_get (Variables|Default|SetArrow _returnvalue_2))
    (Transformation|AttachComponentToComponent _output_get (Variables|/Script/Engine.Character|GetMesh (Variables|Default|GetCharacter)) "RHFS" "KeepWorld" "KeepWorld" "KeepWorld" true)
    (Actor|Tick|SetActorTickEnabled true)
    (bind (_class _value) (CallFunction|GetArrowType))
    (if _value
      (CallFunction|ChangeVisualArrow _class))
    (if (Utilities|Time|IsValidTimerHandle (Variables|Default|GetTimer))
      (Utilities|Time|ClearandInvalidateTimerbyHandle (Variables|Default|GetTimer)))
    (bind _returnvalue_3 (Utilities|Time|SetTimerbyFunctionName 0 "ContinueCharge" 0.01 true))
    (Variables|Default|SetTimer _returnvalue_3)
    (CallFunction|ContinueCharge)
    (Utilities|FlowControl|Delay (Math|Random|RandomFloatinRange 2.0 4.5))
    (Variables|Default|SetHold false)
    (else
      (CallFunction|Fired))))

(event EventGAStop
  (bind _tick_count (Variables|Default|GetTick%20Count))
  (bind _returnvalue (* _tick_count 0.1))
  (bind _returnvalue_2 (* _returnvalue 4e+04))
  ;[1 1 1] Shoots off Arrow. (is called by anim notify)
  (Utilities|IsValid (Variables|Default|GetArrow)
    (:Is%20Valid
      (Transformation|DetachFromActor (Variables|Default|GetArrow) "KeepWorld" "KeepWorld" "KeepWorld")
      (Components|Activation|Activate (Variables|/Game/DATA/Blueprints/Actors/BP_BaseSpell.BP_BaseSpell_C|GetProjectileMovement (Variables|Default|GetArrow)) true)
      (Utilities|Time|ClearandInvalidateTimerbyHandle (Variables|Default|GetTimer))
      (Variables|/Game/DATA/Blueprints/Actors/BP_BaseSpell.BP_BaseSpell_C|SetDamageMultiplier (Variables|Default|GetArrow) (- (+ (* (* (Variables|Default|GetTick%20Count) 0.1) 1.5) (Variables|/Game/DATA/Blueprints/Actors/BP_BaseWeapon.BP_BaseWeapon_C|GetWeaponMultiplierDamage (Default|GetMainWeapon (Variables|Default|GetCombat%20Component)))) 1.0))
      (Default|DamageCalculate (Variables|Default|GetArrow))
      (CallFunction|PlayBowSwingandArrowSound)
      (bind _returnvalue_3 (Default|GetAimTrace (Variables|Default|GetCombat%20Component) (Variables|/Game/DATA/BP_PC.BP_PC_C|GetFollowCamera (Variables|Default|GetCharacter)) (Variables|/Game/DATA/Blueprints/Actors/BP_BaseSpell.BP_BaseSpell_C|GetVisualEffect (Variables|Default|GetArrow)) 6e+03 2e+01 (Variables|/Game/DATA/Blueprints/Components/CombatComponent.CombatComponent_C|GetDraw%20Debug%20Type (Variables|Default|GetCombat%20Component)) false "LHFS" (Variables|Default|GetArrow)))
      (Transformation|SetActorRotation (Variables|Default|GetArrow) (select (Variables|/Game/DATA/Blueprints/Components/CombatComponent.CombatComponent_C|GetIsPlayer (Variables|Default|GetCombat%20Component)) (.rotation _returnvalue_3) (Math|Rotator|MakeRotator (.Roll (Math|Rotator|BreakRotator (.rotation _returnvalue_3))) (+ (.Pitch (Math|Rotator|BreakRotator (.rotation _returnvalue_3))) 1.5) (.Yaw (Math|Rotator|BreakRotator (.rotation _returnvalue_3))))))
      (Game|Components|ProjectileMovement|SetVelocityinLocalSpace (Variables|/Game/DATA/Blueprints/Actors/BP_BaseSpell.BP_BaseSpell_C|GetProjectileMovement (Variables|Default|GetArrow)) (Math|Vector|MakeVector (Math|Float|Clamp(Float) _returnvalue_2 5e+02 _returnvalue_2) 0.0 0.0))
      (Variables|/Script/Engine.ProjectileMovementComponent|SetProjectileGravityScale (Variables|/Game/DATA/Blueprints/Actors/BP_BaseSpell.BP_BaseSpell_C|GetProjectileMovement (Variables|Default|GetArrow)) (CallFunction|GetArrowsWeight))
      (CallFunction|Done 1.0)
      (CallFunction|Reset)
      (Collision|SetCollisionEnabled (Variables|/Game/DATA/Blueprints/Actors/BP_BaseSpell.BP_BaseSpell_C|GetMainProjectileCore (Variables|Default|GetArrow)) "QueryAndPhysics")
      (Variables|Default|SetArrow 0)
      (CallFunction|RemoveArrow)
      (Class|AnimBPI|BowAiming(Message) (Components|SkeletalMesh|GetAnimInstance (Variables|/Script/Engine.Character|GetMesh (Variables|Default|GetCharacter))) false)
      (Actor|Tick|SetActorTickEnabled false)
      (Audio|Components|Audio|Stop (Variables|Default|GetDraw%20Bow%20Sound)))
    (:Is%20Not%20Valid
      ;[1 1 1] End GA
      (Utilities|IsValid (Variables|Default|GetCharacter)
        (:Is%20Valid
          (CallFunction|FloatWeapon false "NewEnumerator2" "NewEnumerator2")
          (Default|RemoveGA (Variables|/Game/DATA/BP_PC.BP_PC_C|GetCombatComponent (Variables|Default|GetCharacter)) (Utilities|GetClass self))
          (Default|SetState (Variables|Default|GetCombat%20Component))
          (Actor|DestroyActor))))))

(event EventDone
  (params (Duration :type Float%20%28single-precision%29))
  ;[1 1 1] End GA
  (Utilities|FlowControl|RetriggerableDelay Duration)
  (Utilities|IsValid (Variables|Default|GetCharacter)
    (:Is%20Valid
      (CallFunction|FloatWeapon false "NewEnumerator2" "NewEnumerator2")
      (Default|RemoveGA (Variables|/Game/DATA/BP_PC.BP_PC_C|GetCombatComponent (Variables|Default|GetCharacter)) (Utilities|GetClass self))
      (Default|SetState (Variables|Default|GetCombat%20Component))
      (Actor|DestroyActor))))

(event EventGAArrowTick
  (params (TickCount :type Float%20%28double-precision%29))
  (bind _skill (Variables|Default|GetSkill))
  (bind (_stamina _mana) (CallFunction|CheckManaStamina _skill))
  ;[1 1 1] Contuinue
  (if (Math|Boolean|ANDBoolean _stamina _mana (Variables|Default|GetDrawling))
    (Variables|Default|SetTick%20Count TickCount)
    (Utilities|IsValid (Variables|/Game/DATA/Blueprints/Actors/Magic/BP_BaseArrowSpell.BP_BaseArrowSpell_C|GetP_ArrowFlash (Variables|Default|GetArrow))
      (:Is%20Valid
        (if (Variables|/Game/DATA/Blueprints/Components/CombatComponent.CombatComponent_C|GetIsPlayer (Variables|Default|GetCombat%20Component))
          (Default|EventCost (Variables|Default|GetStats%20Component) (Variables|Default|GetSkill)))
        (Components|Activation|Activate (Variables|/Game/DATA/Blueprints/Actors/Magic/BP_BaseArrowSpell.BP_BaseArrowSpell_C|GetP_ArrowFlash (Variables|Default|GetArrow)) true))
      (:Is%20Not%20Valid
        (Utilities|Time|ClearandInvalidateTimerbyHandle (Variables|Default|GetTimer))))
    (else
      (Default|OOMCheck (Variables|Default|GetStats%20Component) (Math|Conversions|ToFloat(Integer) (.Stamina%20Cost (Default|GetSkillStats (Variables|Default|GetStats%20Component) (Variables|Default|GetSkill)))))
      (Variables|Default|SetDrawling false))))

(event EventTick
  (params (DeltaSeconds :type Float%20%28single-precision%29))
  ;[1 1 1] Spawn
  (Utilities|IsValid (Variables|Default|GetCharacter)
    (:Is%20Valid
      (Default|RotatetoCamera (Variables|Default|GetTargetingComponent) 0.5))
    (:Is%20Not%20Valid
      (Actor|DestroyActor))))

(fn ConstructionScript
  (|CallParentFunction))

(fn Hold?
  (return (and (Utilities|Enum|Equal(Enum) (.State (Default|GetKeyStates (Variables|Default|GetCharacter) (Variables|Default|GetKeyIndex))) "NewEnumerator1") (Default|GetCurrentStateNotEqualAny (Variables|Default|GetCombat%20Component) "(GameplayTags=((TagName=\"Character.Action.Skill/Magic.Jump\"),(TagName=\"Character.State.Dodging\"),(TagName=\"Character.Action.Stuned\"),(TagName=\"Character.State.Attacking\"),(TagName=\"Character.State.Dead\"),(TagName=\"Character.State.Disabled\")))"))))

(fn PullAnimation
  (params (DrawSpeed :type Float%20%28double-precision%29))
  (bind _stats_component (Variables|Default|GetStats%20Component))
  (bind _value (Default|GetSubStats _stats_component "NewEnumerator19"))
  (bind _returnvalue (- DrawSpeed 1.0))
  (bind _returnvalue_2 (+ _value _returnvalue))
  (Animation|PlayAnimMontage (Variables|Default|GetCharacter) (Utilities|Array|Get(acopy) (Variables|Default|GetAttackMontages)) _returnvalue_2 "None")
  (Animation|Montage|MontagePlay (Components|SkeletalMesh|GetAnimInstance (.ItemSkeletalMesh (CallFunction|GetBow))) "/Game/DATA/Animations/Bow/BowSkelAnimations/PullAndHold_Montage.PullAndHold_Montage" _returnvalue_2 "MontageLength" 0.0 true)
  (bind _asbp_base_bow (Utilities|Casting|CastToBP_BaseBow (.ReturnValue (CallFunction|GetBow)))
    (:then
      (bind _output_get (Variables|Default|SetDraw%20Bow%20Sound (Variables|/Game/DATA/Blueprints/Actors/BP_BaseBow.BP_BaseBow_C|GetDrawBowSound _asbp_base_bow)))
      (Audio|Components|Audio|SetPitchMultiplier _output_get _returnvalue_2)
      (Audio|Components|Audio|Play _output_get 0.0))
    (:CastFailed
      _))
  (return))

(fn SetCost
  (bind _skill (Variables|Default|GetSkill))
  (bind _stats_component (Variables|Default|GetStats%20Component))
  (bind (_combat_types _mana_cost _stamina_cost) (Default|GetSkillStats _stats_component _skill))
  (Default|SetActionCost (Variables|Default|GetStats%20Component) (Variables|Default|GetSkill) (Math|Conversions|ToFloat(Integer) (Math|Integer|Clamp(Integer) _stamina_cost 1 _stamina_cost)) (Math|Conversions|ToFloat(Integer) (Math|Integer|Clamp(Integer) _mana_cost 0 _mana_cost))))

(fn PlayBowSwingandArrowSound
  (Components|Activation|Activate (Variables|/Game/DATA/Blueprints/Actors/BP_BaseWeapon.BP_BaseWeapon_C|GetImpactSound (select (Utilities|Enum|Equal(Enum) (Variables|/Game/DATA/Blueprints/Actors/BP_BaseWeapon.BP_BaseWeapon_C|GetTwoHandedCombatType (Default|GetMainWeapon (Variables|Default|GetCombat%20Component))) "NewEnumerator5") (Default|GetMainWeapon (Variables|Default|GetCombat%20Component)) (Default|GetOffHandedWeapon (Variables|Default|GetCombat%20Component)))) true)
  (Components|Activation|Activate (Variables|/Game/DATA/Blueprints/Actors/BP_BaseSpell.BP_BaseSpell_C|GetFlySound (Variables|Default|GetArrow)) true)
  (Components|Activation|Activate (Variables|/Game/DATA/Blueprints/Actors/BP_BaseSpell.BP_BaseSpell_C|GetTrail (Variables|Default|GetArrow)) true))

(fn SetRotation
  (bind _arrow (Variables|Default|GetArrow))
  (bind _character (Variables|Default|GetCharacter))
  (bind _returnvalue (Transformation|GetActorRotation _character))
  (bind _returnvalue_2 (Default|GetAimTrace (Variables|Default|GetCombat%20Component) (Variables|/Game/DATA/BP_PC.BP_PC_C|GetFollowCamera (Variables|Default|GetCharacter)) (Variables|/Game/DATA/Blueprints/Actors/BP_BaseSpell.BP_BaseSpell_C|GetVisualEffect _arrow) 6e+03 2e+01 (Variables|/Game/DATA/Blueprints/Components/CombatComponent.CombatComponent_C|GetDraw%20Debug%20Type (Variables|Default|GetCombat%20Component)) false "LHFS" _arrow))
  (Transformation|SetActorRotation (Variables|Default|GetCharacter) (Math|Rotator|MakeRotator (.Roll (Math|Rotator|BreakRotator _returnvalue)) 0.0 (.yaw (Math|Interpolation|RInterpTo _returnvalue (.rotation _returnvalue_2) (Utilities|Time|GetWorldDeltaSeconds) (Variables|Default|GetTargetRotationInterp%20Speed))))))

(fn IsThereAnyArrows
  (bind _keys (Utilities|Map|Keys (Variables|/Game/DATA/Blueprints/Components/EquipmentComponet.EquipmentComponet_C|GetEquiped (Variables|/Game/DATA/BP_PC.BP_PC_C|GetEquipmentComponet (Variables|Default|GetCharacter)))))
  (for _array_element _keys
    (if (Utilities|Enum|Equal(Enum) (.EquipType (Utilities|Struct|BreakS_EquippedItemInfo (.Value (Utilities|Map|Find (Variables|/Game/DATA/Blueprints/Components/EquipmentComponet.EquipmentComponet_C|GetEquiped (Variables|/Game/DATA/BP_PC.BP_PC_C|GetEquipmentComponet (Variables|Default|GetCharacter))) _array_element)))) "NewEnumerator29")
      (return true (.EquipedItem (Utilities|Struct|BreakS_EquippedItemInfo (.Value (Utilities|Map|Find (Variables|/Game/DATA/Blueprints/Components/EquipmentComponet.EquipmentComponet_C|GetEquiped (Variables|/Game/DATA/BP_PC.BP_PC_C|GetEquipmentComponet (Variables|Default|GetCharacter))) _array_element)))))))
  (return false 0))

(fn RemoveArrow
  (bind _character (Variables|Default|GetCharacter))
  (bind _character_2 (Variables|Default|GetCharacter))
  (bind _inventory (Variables|/Game/DATA/BP_PC.BP_PC_C|GetInventory _character))
  (bind _inventory_2 (Variables|/Game/DATA/BP_PC.BP_PC_C|GetInventory _character_2))
  (bind _mainwidget (Variables|/Game/DATA/Blueprints/Actors/Inventory/BP_Inventory.BP_Inventory_C|GetMainWidget _inventory_2))
  (bind _arrowslots (Variables|/Game/DATA/Blueprints/Actors/Inventory/BP_Inventory.BP_Inventory_C|GetArrowSlots _inventory))
  (bind _cw_equipmentwidget (Variables|/Game/DATA/UI/Inventory/WBP_MainWidget.WBP_MainWidget_C|GetCW_EquipmentWidget _mainwidget))
  (bind _cw_arrows (Variables|/Game/DATA/UI/Inventory/CW_EquipmentWidget.CW_EquipmentWidget_C|GetCW_Arrows _cw_equipmentwidget))
  (if (Variables|/Game/DATA/Blueprints/Components/CombatComponent.CombatComponent_C|GetIsPlayer (Variables|Default|GetCombat%20Component))
    (Default|RemoveItematIndexAlt _inventory 0 1 false _arrowslots)
    (if (Default|IsSlotEmptyAlt _inventory 0 _arrowslots)
      (Utilities|IsValid _cw_arrows
        (:Is%20Valid
          (Default|UnequipItem _cw_arrows false)
          (return)))
      (else
        (return)))
    (else
      (return))))

(fn GetArrowType
  (bind _keys (Utilities|Map|Keys (Variables|/Game/DATA/Blueprints/Components/EquipmentComponet.EquipmentComponet_C|GetEquiped (Variables|/Game/DATA/BP_PC.BP_PC_C|GetEquipmentComponet (Variables|Default|GetCharacter)))))
  (for _array_element _keys
    (if (Utilities|Enum|Equal(Enum) (.EquipType (Utilities|Struct|BreakS_EquippedItemInfo (.Value (Utilities|Map|Find (Variables|/Game/DATA/Blueprints/Components/EquipmentComponet.EquipmentComponet_C|GetEquiped (Variables|/Game/DATA/BP_PC.BP_PC_C|GetEquipmentComponet (Variables|Default|GetCharacter))) _array_element)))) "NewEnumerator29")
      (return _array_element true)))
  (return 0 false))

(fn ChangeVisualArrow
  (params (Item%20Class :type BP%20Master%20Item%20Class%20Reference))
  (bind _arrow (Variables|Default|GetArrow))
  (bind _output_get (Variables|/Game/DATA/Blueprints/Actors/Magic/BP_BaseArrowSpell.BP_BaseArrowSpell_C|SetItem%20Class _arrow Item%20Class))
  (Components|StaticMesh|SetStaticMesh (Variables|/Game/DATA/Blueprints/Actors/BP_BaseSpell.BP_BaseSpell_C|GetVisualEffect _arrow) (Utilities|GetClassDefaults _output_get)))

(fn GetArrowsWeight
  (bind _equiped_arrows (Variables|Default|GetEquiped%20Arrows))
  (bind _substatsbuff (Variables|/Game/DATA/Blueprints/Actors/BP_MasterItem.BP_MasterItem_C|GetSubStatsBuff _equiped_arrows))
  (bind (_value _returnvalue) (Utilities|Map|Find _substatsbuff "NewEnumerator32"))
  (return (select _returnvalue _value 1.0)))

(fn GetBow
  (bind _combat_component (Variables|Default|GetCombat%20Component))
  (bind _returnvalue (Default|GetMainWeapon _combat_component))
  (bind _equipedoffhand (Default|GetOffHandedWeapon _combat_component))
  (bind _twohandedcombattype (Variables|/Game/DATA/Blueprints/Actors/BP_BaseWeapon.BP_BaseWeapon_C|GetTwoHandedCombatType _returnvalue))
  (bind _returnvalue_2 (Utilities|Enum|Equal(Enum) _twohandedcombattype "NewEnumerator5"))
  (bind _returnvalue_3 (select _returnvalue_2 _returnvalue _equipedoffhand))
  (return (Variables|/Game/DATA/Blueprints/Actors/BP_MasterItem.BP_MasterItem_C|GetItemSkeletalMesh _returnvalue_3) _returnvalue_3))