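; Player fireball ability actor that charges a projectile while the key is held, then fires it along an aim trace.
; Montages drive spawn and launch, with the fireball attached to the character during charging.
; A looping timeline adds damage and grows it up to the skill's Power while stamina and mana suffice, then holds until release or jump.
; A retriggerable delay acts as watchdog, removing and destroying the ability.
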(event Custom|ContinueCharge
  (bind _stats_component (Variables|Default|GetStats%20Component))
  (bind _stats_component_2 (Variables|Default|GetStats%20Component))
  (bind _stats_component_3 (Variables|Default|GetStats%20Component))
  (bind (_combat_types _mana_cost _stamina_cost) (Default|GetSkillStats _stats_component_2 "(TagName=\"Character.Action.Skill/Magic.FireBall\")"))
  (bind (_combat_types_2 _mana_cost_2 _stamina_cost_2 _skill_xp _level_up_cost _skill_xpspent _skill_level _available_points _power) (Default|GetSkillStats _stats_component_3 "(TagName=\"Character.Action.Skill/Magic.FireBall\")"))
  ;[1 1 1] Grow
  (if (Utilities|Enum|Equal(Enum) (.State (Default|GetKeyStates (Variables|Default|GetCharacter) (Variables|Default|GetKeyIndex))) "NewEnumerator1")
    (Default|SetState (Variables|Default|GetCombat%20Component) "(TagName=\"Character.State.GenralActionState\")")
    (CallFunction|Done 5.0)
    (if (and (Default|StatGreaterThen _stats_component "NewEnumerator2" (Math|Conversions|ToFloat(Integer) _stamina_cost)) (Default|StatGreaterThen _stats_component "NewEnumerator4" (Math|Conversions|ToFloat(Integer) _mana_cost)))
      (Default|SetCurrentAction (Variables|Default|GetCombat%20Component) "(TagName=\"Character.Action.Skill/Magic.FireBall\")")
      (if (> _power (Variables|Default|GetCurrentPower))
        (Math|Float|IncrementFloat (Variables|Default|GetChargePower)
          (:%20%20
            (bind _onesec (Timeline|FireBallTimer PlayFromStart)
              (:Update
                (if (CallFunction|Hold?)
                  (Utilities|IsValid (Variables|Default|GetFireBall)
                    (:Is%20Valid
                      (Default|AddDamage (Variables|Default|GetFireBall) (Math|Float|Lerp (Variables|Default|GetCurrentPower) (Variables|Default|GetChargePower) _onesec))
                      (CallFunction|Done 5.0)
                      (Default|Grow (Variables|Default|GetFireBall))))
                  (else
                    (CallFunction|Launch))))
              (:Finished
                (Variables|Default|SetCurrentPower (Variables|Default|GetChargePower))
                (CallFunction|ContinueCharge)))))
        (else
          (CallFunction|HoldCheck)))
      (else
        (Default|OOMCheck (Variables|Default|GetStats%20Component) (Math|Conversions|ToFloat(Integer) _mana_cost_2))
        (CallFunction|HoldCheck)))
    (else
      (CallFunction|Launch))))

(event Custom|Launch
  ;[1 1 1] Launch the FireBall
  (if (Variables|Default|GetCharging)
    (Variables|Default|SetCharging false)
    (if (Default|GetCurrentStateNotEqualAny (Variables|Default|GetCombat%20Component) "(GameplayTags=((TagName=\"Character.Action.Skill/Magic.Jump\"),(TagName=\"Character.State.Dodging\"),(TagName=\"Character.Action.Stuned\"),(TagName=\"Character.State.Attacking\"),(TagName=\"Character.State.Dead\"),(TagName=\"Character.State.Disabled\")))")
      (Default|RotatetoTarget (Variables|Default|GetCharacter))
      (Default|PerformComboAction (Variables|Default|GetCombat%20Component) false (Variables|Default|GetAttackMontages2))
      (else
        (CallFunction|Fired)))))

(event Custom|HoldCheck
  ;[1 1 1] If charge complete or OOMed this keeps fire ball held to launched
  (if (CallFunction|Hold?)
    (Utilities|FlowControl|Delay 0.1)
    (CallFunction|HoldCheck)
    (CallFunction|Done 5.0)
    (else
      (CallFunction|Launch))))

(event Custom|fired
  (bind _fireball (Variables|Default|GetFireBall))
  (bind _fireball_2 (Variables|Default|GetFireBall))
  ;[1 1 1] Shoots off the fire ball. (is called by anim notify)
  (Utilities|IsValid (Variables|Default|GetFireBall)
    (:Is%20Valid
      (Transformation|DetachFromActor (Variables|Default|GetFireBall) "KeepWorld" "KeepWorld" "KeepWorld")
      (bind _returnvalue (Default|GetAimTrace (Variables|Default|GetCombat%20Component) (Variables|/Game/DATA/BP_PC.BP_PC_C|GetFollowCamera (Variables|Default|GetCharacter)) (Variables|/Game/DATA/Blueprints/Actors/BP_BaseSpell.BP_BaseSpell_C|GetVisualEffect _fireball) 6e+03 2e+01 (Variables|/Game/DATA/Blueprints/Components/CombatComponent.CombatComponent_C|GetDraw%20Debug%20Type (Variables|Default|GetCombat%20Component)) false "RHFS" _fireball))
      (Transformation|SetActorRotation _fireball_2 (.rotation _returnvalue))
      (Game|Components|ProjectileMovement|SetVelocityinLocalSpace (Variables|/Game/DATA/Blueprints/Actors/BP_BaseSpell.BP_BaseSpell_C|GetProjectileMovement _fireball_2) "3000.000000,0.000000,0.000000")
      (CallFunction|Done 5.0))
    (:Is%20Not%20Valid
      ;[1 1 1] End GA
      (CallFunction|FloatWeapon false "NewEnumerator2" "NewEnumerator2")
      (Default|RemoveGA (Variables|/Game/DATA/BP_PC.BP_PC_C|GetCombatComponent (Variables|Default|GetCharacter)) (Utilities|GetClass self))
      (Actor|DestroyActor))))

(event EventBeginPlay
  (|CallParentFunction) ; This node is disabled and will not be called.\nDrag off pins to build functionality.
)

(event Collision|EventActorBeginOverlap
  (params (OtherActor :type Actor%20Object%20Reference)))

(event EventTick
  (params (DeltaSeconds :type Float%20%28single-precision%29)))

(event EventGAStart
  (bind _stats_component (Variables|Default|GetStats%20Component))
  (bind _stats_component_2 (Variables|Default|GetStats%20Component))
  (bind (_combat_types _mana_cost _stamina_cost) (Default|GetSkillStats _stats_component_2 "(TagName=\"Character.Action.Skill/Magic.FireBall\")"))
  ;[1 1 1] Start
  (if (Math|Boolean|ANDBoolean (Default|StatGreaterThen _stats_component "NewEnumerator2" (Math|Conversions|ToFloat(Integer) _stamina_cost)) (Default|StatGreaterThen _stats_component "NewEnumerator4" (Math|Conversions|ToFloat(Integer) _mana_cost)) (Default|CanProformCombat (Variables|Default|GetCombat%20Component)))
    (Default|RotatetoTarget (Variables|Default|GetCharacter))
    (Variables|Default|SetCurrentPower 0.0)
    (Variables|Default|SetChargePower 0.0)
    (Default|PerformComboAction (Variables|Default|GetCombat%20Component) false (Variables|Default|GetAttackMontages))
    (Default|SetState (Variables|Default|GetCombat%20Component) "(TagName=\"Character.State.GenralActionState\")")
    (Variables|Default|SetCharging true)
    (CallFunction|Done 5.0)
    (else
      (Default|OOMCheck (Variables|Default|GetStats%20Component) (Math|Conversions|ToFloat(Integer) (.Stamina%20Cost (Default|GetSkillStats (Variables|Default|GetStats%20Component) "(TagName=\"Character.Action.Skill/Magic.FireBall\")"))))
      (CallFunction|Done 5.0))))

(event EventActivateComboSkill
  (params (Hand :type E_Handed%20Enum :default "NewEnumerator0"))
  (bind _stats_component (Variables|Default|GetStats%20Component))
  (bind _character (Variables|Default|GetCharacter))
  (bind _stats_component_2 (Variables|Default|GetStats%20Component))
  (bind _character_2 (Variables|Default|GetCharacter))
  (bind _character_3 (Variables|Default|GetCharacter))
  (bind _effectiveness (Default|GetSkillStats _stats_component "(TagName=\"Character.Action.Skill/Magic.FireBall\")"))
  (bind (_combat_types _mana_cost _stamina_cost) (Default|GetSkillStats _stats_component_2 "(TagName=\"Character.Action.Skill/Magic.FireBall\")"))
  (bind _mesh (Variables|/Script/Engine.Character|GetMesh _character_3))
  ;[1 1 1] Spawn
  (if (CallFunction|IsGAActive)
    (if (Variables|Default|GetCharging)
      (CallFunction|FloatWeapon true "NewEnumerator2" "NewEnumerator2")
      (Default|SetActionCost (Variables|Default|GetStats%20Component) "(TagName=\"Character.Action.Skill/Magic.FireBall\")" (Math|Conversions|ToFloat(Integer) _stamina_cost) (Math|Conversions|ToFloat(Integer) _mana_cost))
      (CallFunction|Done 5.0)
      (Default|SetState (Variables|Default|GetCombat%20Component) "(TagName=\"Character.State.GenralActionState\")")
      (Utilities|IsValid (Variables|Default|GetFireBall)
        (:Is%20Valid
          (Variables|Default|SetLuanchedFireBall (Variables|Default|GetFireBall)))
        (:Is%20Not%20Valid
          _))
      (bind _returnvalue (Default|GetAimTrace (Variables|Default|GetCombat%20Component) (Variables|/Game/DATA/BP_PC.BP_PC_C|GetFollowCamera _character_2) (Variables|/Script/Engine.Character|GetMesh _character_2) 6e+03 2e+01 (Variables|/Game/DATA/Blueprints/Components/CombatComponent.CombatComponent_C|GetDraw%20Debug%20Type (Variables|Default|GetCombat%20Component)) true "RHFS" (Variables|Default|GetCharacter)))
      (bind _returnvalue_2 (Game|SpawnActorfromClass "/Game/DATA/Blueprints/Actors/Magic/BP_FireBallSpell.BP_FireBallSpell_C" (Math|Transform|MakeTransform (+ (+ (/ (+ (Transformation|GetSocketLocation _mesh "RHFS") (Transformation|GetSocketLocation _mesh "LHFS")) 2.0) (* (Transformation|GetActorForwardVector _character_3) 5e+01)) "0.000000,0.000000,50.000000") (.rotation _returnvalue) "1.000000,1.000000,1.000000") "Undefined" "MultiplyWithRoot" _character 0.0 _effectiveness 2e+04 0.0 _character _effectiveness true "(TagName=\"Character.Action.Skill/Magic.FireBall\")" false 0.0 _character))
      (bind _output_get (Variables|Default|SetFireBall _returnvalue_2))
      (Transformation|AttachActorToActor _output_get (Variables|Default|GetCharacter) "None" "KeepWorld" "KeepWorld" "KeepWorld" true)
      (CallFunction|ContinueCharge)
      (else
        (CallFunction|Fired)))))

(event EventGAStop
  (bind _fireball (Variables|Default|GetFireBall))
  (bind _fireball_2 (Variables|Default|GetFireBall))
  ;[1 1 1] Shoots off the fire ball. (is called by anim notify)
  (Utilities|IsValid (Variables|Default|GetFireBall)
    (:Is%20Valid
      (Transformation|DetachFromActor (Variables|Default|GetFireBall) "KeepWorld" "KeepWorld" "KeepWorld")
      (bind _returnvalue (Default|GetAimTrace (Variables|Default|GetCombat%20Component) (Variables|/Game/DATA/BP_PC.BP_PC_C|GetFollowCamera (Variables|Default|GetCharacter)) (Variables|/Game/DATA/Blueprints/Actors/BP_BaseSpell.BP_BaseSpell_C|GetVisualEffect _fireball) 6e+03 2e+01 (Variables|/Game/DATA/Blueprints/Components/CombatComponent.CombatComponent_C|GetDraw%20Debug%20Type (Variables|Default|GetCombat%20Component)) false "RHFS" _fireball))
      (Transformation|SetActorRotation _fireball_2 (.rotation _returnvalue))
      (Game|Components|ProjectileMovement|SetVelocityinLocalSpace (Variables|/Game/DATA/Blueprints/Actors/BP_BaseSpell.BP_BaseSpell_C|GetProjectileMovement _fireball_2) "3000.000000,0.000000,0.000000")
      (CallFunction|Done 5.0))
    (:Is%20Not%20Valid
      ;[1 1 1] End GA
      (CallFunction|FloatWeapon false "NewEnumerator2" "NewEnumerator2")
      (Default|RemoveGA (Variables|/Game/DATA/BP_PC.BP_PC_C|GetCombatComponent (Variables|Default|GetCharacter)) (Utilities|GetClass self))
      (Actor|DestroyActor))))

(event EventDone
  (params (Duration :type Float%20%28single-precision%29))
  ;[1 1 1] End GA
  (Utilities|FlowControl|RetriggerableDelay Duration)
  (CallFunction|FloatWeapon false "NewEnumerator2" "NewEnumerator2")
  (Default|RemoveGA (Variables|/Game/DATA/BP_PC.BP_PC_C|GetCombatComponent (Variables|Default|GetCharacter)) (Utilities|GetClass self))
  (Actor|DestroyActor))

(fn ConstructionScript
  (|CallParentFunction))

(fn Hold?
  (return (and (Utilities|Enum|Equal(Enum) (.State (Default|GetKeyStates (Variables|Default|GetCharacter) (Variables|Default|GetKeyIndex))) "NewEnumerator1") (Default|GetCurrentStateNotEqualAny (Variables|Default|GetCombat%20Component) "(GameplayTags=((TagName=\"Character.Action.Skill/Magic.Jump\"),(TagName=\"Character.State.Dodging\"),(TagName=\"Character.Action.Stuned\"),(TagName=\"Character.State.Attacking\"),(TagName=\"Character.State.Dead\"),(TagName=\"Character.State.Disabled\")))"))))