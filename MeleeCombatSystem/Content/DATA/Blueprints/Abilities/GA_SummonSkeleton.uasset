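; Skeleton summon ability that places armed skeleton NPCs where the player aims while holding the key.
; A looping timer sphere-traces along the camera, moving a preview whose count follows skill Effectiveness and box-checking each spot.
; Releasing after enough hold ticks plays a cast montage whose notify pays costs, grants XP, equips summon equipment and spawns skeletons leveled by Power.
; Despawn clears prior summons; retriggerable Done delays remove the ability.
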(event Custom|GetSpawnTarget
  ;[1 1 1] Check if still charging
  (if (Utilities|Enum|Equal(Enum) (.State (Default|GetKeyStates (Variables|Default|GetCharacter) (Variables|Default|GetKeyIndex))) "NewEnumerator1")
    (CallFunction|GetSpawnPoint)
    (else
      (Utilities|Time|ClearandInvalidateTimerbyHandle (Variables|Default|GetSummonTimer))
      (if (> (Variables|Default|GetHeldTime) 50)
        (CallFunction|SpawnSkeleton)
        (else
          (CallFunction|Despawn))))))

(event Custom|SpawnSkeleton
  ;[1 1 1] Summon
  (Actor|DestroyActor (Variables|Default|GetSpawnPreview))
  (if (Default|CanProformCombat (Variables|Default|GetCombat%20Component))
    (CallFunction|Despawn)
    (CallFunction|FloatWeapon true "NewEnumerator2" "NewEnumerator4")
    (CallFunction|Done 1e+01)
    (Animation|Montage|PlayMontage (Variables|/Script/Engine.Character|GetMesh (Variables|Default|GetCharacter)) "/Game/DATA/Animations/Magic/Summon_Casting_Montage.Summon_Casting_Montage" (Default|GetSubStats (Variables|Default|GetStats%20Component) "NewEnumerator19")
      (:then
        (bind _returnvalue (Audio|SpawnSoundatLocation "/Game/DATA/SoundFX/Earth/BuildingRumble/SC_RockRumble.SC_RockRumble" (Transformation|GetActorLocation (Variables|Default|GetCharacter)) "0, 0, 0" 1.0 1.0 0.0 0 0))
        (Variables|Default|SetSound _returnvalue))
      (:OnNotifyBegin
        (CallFunction|Cost)
        (Utilities|FlowControl|Sequence
          (:then_0
            (for _array_element (Variables|Default|GetSpawnLocation)
              (bind _returnvalue_2 (Game|SpawnActorfromClass "/Game/DATA/Blueprints/Actors/Utility/BP_SpawnActors.BP_SpawnActors_C" (Math|Transform|MakeTransform (+ _array_element "0.000000,0.000000,150.000000") (Transformation|GetWorldRotation (Variables|/Game/DATA/BP_PC.BP_PC_C|GetFollowCamera (Variables|Default|GetCharacter))) "1.000000,1.000000,1.000000") "AdjustIfPossibleButAlwaysSpawn" "MultiplyWithRoot" 0 (Utilities|Array|MakeArray "/Game/DATA/Blueprints/Actors/Weapons/BP_CrustedBlade.BP_CrustedBlade_C" "/Game/DATA/Blueprints/Actors/Weapons/BP_OldShield.BP_OldShield_C") "NewEnumerator2" (Math|Float|Truncate (.Power (Default|GetSkillStats (Variables|Default|GetStats%20Component) (Variables|Default|GetSkill)))) "Summon Skeleton" 0 0 true true true true false 0 0 true false true 0 true 1 false true false false 0))
              (Variables|/Game/DATA/Blueprints/Actors/Utility/BP_SpawnActors.BP_SpawnActors_C|SetClass _returnvalue_2 (Variables|Default|GetSummonClass))
              (Utilities|IsThisValid _returnvalue_2 5.0
                (:Is%20Valid
                  (Utilities|Array|Add (Variables|Default|GetSummonSkeleton) (Variables|/Game/DATA/Blueprints/Actors/Utility/BP_SpawnActors.BP_SpawnActors_C|GetCharacter _returnvalue_2))))))
          (:then_1
            (Audio|Components|Audio|FadeOut (Variables|Default|GetSound) 2.0 0.0 "Linear" :!class /Script/Engine.AudioComponent)))))
    (else
      (Utilities|Array|Clear (Variables|Default|GetSpawnLocation)))))

(event Custom|GetSpawnPoint
  (bind _character (Variables|Default|GetCharacter))
  (bind _mesh (Variables|/Script/Engine.Character|GetMesh _character))
  (bind _returnvalue (Transformation|GetWorldLocation _mesh))
  ;[1 1 1] Get Spawn Point
  (Math|Integer|IncrementInt (Variables|Default|GetHeldTime)
    (:%20%20
      (bind (_outhit _returnvalue_2) (Collision|SphereTraceForObjects (+ _returnvalue "0.000000,0.000000,150.000000") (+ _returnvalue (* (Math|Vector|GetForwardVector (Variables|/Game/DATA/BP_PC.BP_PC_C|GetFollowCamera _character)) 2.5e+03)) 2e+01 (Utilities|Array|MakeArray "ObjectTypeQuery1" "ObjectTypeQuery6" "ObjectTypeQuery11" "ObjectTypeQuery9" "ObjectTypeQuery5") false (Utilities|Array|MakeArray (Variables|Default|GetCharacter)) "None"))
      (if _returnvalue_2
        (if (Utilities|IsValid (Variables|Default|GetSpawnPreview))
          (CallFunction|Done 3.0)
          (Transformation|SetActorLocation (Variables|Default|GetSpawnPreview) (.ImpactPoint (Collision|BreakHitResult _outhit)) false true)
          (Transformation|SetActorRotation (Variables|Default|GetSpawnPreview) (Math|Rotator|MakeRotator 0.0 0.0 (+ (.yaw (Transformation|GetWorldRotation (Variables|/Game/DATA/BP_PC.BP_PC_C|GetFollowCamera (Variables|Default|GetCharacter)))) -9e+01)))
          (if (CallFunction|IsPrivewOverlaping?)
            (CallFunction|SetSpawnLocs)
            (Default|ChangeColor (Variables|Default|GetSpawnPreview) true)
            (else
              (Default|ChangeColor (Variables|Default|GetSpawnPreview) false)))
          (else
            (bind _returnvalue_3 (Game|SpawnActorfromClass "/Game/DATA/Blueprints/Actors/Utility/BP_PreviewSpawn.BP_PreviewSpawn_C" (Math|Transform|MakeTransform (.ImpactPoint (Collision|BreakHitResult _outhit)) (Math|Rotator|MakeRotator 0.0 0.0 (+ (.yaw (Transformation|GetWorldRotation (Variables|/Game/DATA/BP_PC.BP_PC_C|GetFollowCamera (Variables|Default|GetCharacter)))) -9e+01)) "1.000000,1.000000,1.000000") "Undefined" "MultiplyWithRoot" 0 (Math|Float|Truncate (+ (.Effectiveness (Default|GetSkillStats (Variables|Default|GetStats%20Component) (Variables|Default|GetSkill))) 0.1)) 0))
            (bind _output_get (Variables|Default|SetSpawnPreview _returnvalue_3))
            (Utilities|FlowControl|Delay 0.1)
            (Default|Spawn _output_get)))))))

(event Custom|Despawn
  (bind _spawnpreview (Variables|Default|GetSpawnPreview))
  ;[1 1 1] Despawn
  (Utilities|IsValid _spawnpreview
    (:Is%20Valid
      (Actor|DestroyActor _spawnpreview))
    (:Is%20Not%20Valid
      _))
  (Default|UnequipClass (Variables|/Game/DATA/BP_PC.BP_PC_C|GetEquipmentComponet (Variables|Default|GetCharacter)) (Variables|Default|GetSummonEquipment))
  (bind _outactors (Actor|GetAllActorsOfClass (Variables|Default|GetSummonClass)))
  (for _array_element _outactors
    (Class|CombatBPI|Reset(Message) _array_element)))

(event EventBeginPlay
  (|CallParentFunction) ; This node is disabled and will not be called.\nDrag off pins to build functionality.
)

(event Collision|EventActorBeginOverlap
  (params (OtherActor :type Actor%20Object%20Reference)))

(event EventTick
  (params (DeltaSeconds :type Float%20%28single-precision%29)))

(event EventGAStart
  (bind _skill (Variables|Default|GetSkill))
  (bind (_stamina _mana) (CallFunction|CheckManaStamina _skill))
  ;[1 1 1] Start
  (if (Math|Boolean|ANDBoolean _stamina _mana (Default|CanProformCombat (Variables|Default|GetCombat%20Component)))
    (Default|RotatetoTarget (Variables|Default|GetCharacter))
    (bind _returnvalue (Utilities|Time|SetTimerbyFunctionName 0 "GetSpawnTarget" 0.01 true))
    (Variables|Default|SetSummonTimer _returnvalue)
    (Variables|Default|SetHeldTime 0)
    (else
      (Default|OOMCheck (Variables|Default|GetStats%20Component) (Math|Conversions|ToFloat(Integer) (.Stamina%20Cost (Default|GetSkillStats (Variables|Default|GetStats%20Component) (Variables|Default|GetSkill)))))
      (CallFunction|Done 3.0)
      (CallFunction|Despawn))))

(event EventDone
  (params (Duration :type Float%20%28single-precision%29))
  (bind _spawnpreview (Variables|Default|GetSpawnPreview))
  ;[1 1 1] Done self delete
  (Utilities|FlowControl|RetriggerableDelay Duration)
  (CallFunction|FloatWeapon false "NewEnumerator2" "NewEnumerator0")
  (Default|RemoveGA (Variables|/Game/DATA/BP_PC.BP_PC_C|GetCombatComponent (Variables|Default|GetCharacter)) "GA_SummonSkeleton_C")
  (Utilities|IsValid _spawnpreview
    (:Is%20Valid
      (Actor|DestroyActor _spawnpreview))
    (:Is%20Not%20Valid
      _))
  (Actor|DestroyActor))

(fn ConstructionScript
  (|CallParentFunction))

(fn IsPrivewOverlaping?
  (for _array_element (Variables|/Game/DATA/Blueprints/Actors/Utility/BP_PreviewSpawn.BP_PreviewSpawn_C|GetPreviews (Variables|Default|GetSpawnPreview))
    (bind _returnvalue (Collision|BoxTraceByChannel (.Origin (Collision|GetComponentBounds _array_element)) (.Origin (Collision|GetComponentBounds _array_element)) (* (.BoxExtent (Collision|GetComponentBounds _array_element)) 0.8) "0, 0, 0" "TraceTypeQuery4" false (Utilities|Array|MakeArray (Variables|Default|GetSpawnPreview)) "None" true "(R=1.000000,G=0.000000,B=0.000000,A=1.000000)" "(R=0.000000,G=1.000000,B=0.000000,A=1.000000)" 0.2))
    (if _returnvalue
      (return false)))
  (return true))

(fn SetSpawnLocs
  (Utilities|Array|Clear (Variables|Default|GetSpawnLocation))
  (for _array_element (Variables|/Game/DATA/Blueprints/Actors/Utility/BP_PreviewSpawn.BP_PreviewSpawn_C|GetPreviews (Variables|Default|GetSpawnPreview))
    (Utilities|Array|Add (Variables|Default|GetSpawnLocation) (Transformation|GetWorldLocation _array_element))))

(fn Cost
  (bind _stats_component (Variables|Default|GetStats%20Component))
  (bind _skill (Variables|Default|GetSkill))
  (bind _skill_2 (Variables|Default|GetSkill))
  (bind _summonequipment (Variables|Default|GetSummonEquipment))
  (bind (_combat_types _mana_cost _stamina_cost _skill_xp _level_up_cost _skill_xpspent _skill_level _available_points _power _effectiveness) (Default|GetSkillStats _stats_component _skill))
  (if (not (.ReturnValue (Default|IsClassEquiped (Variables|/Game/DATA/BP_PC.BP_PC_C|GetEquipmentComponet (Variables|Default|GetCharacter)) (Variables|Default|GetSummonEquipment))))
    _
    (else
      (CallFunction|Despawn)))
  (Default|SetActionCost (Variables|Default|GetStats%20Component) (Variables|Default|GetSkill) (Math|Conversions|ToFloat(Integer) _stamina_cost) (Math|Conversions|ToFloat(Integer) _mana_cost))
  (Default|SetCurrentAction (Variables|Default|GetCombat%20Component) _skill_2)
  (Default|ModifySkillXP (Variables|Default|GetStats%20Component) _skill_2 (Math|Float|Truncate (* (+ _power _effectiveness) 1e+01)) true)
  (bind _newequip (Default|EquipItem (Variables|/Game/DATA/BP_PC.BP_PC_C|GetEquipmentComponet (Variables|Default|GetCharacter)) _summonequipment "NewEnumerator7" (Utilities|GetClassDefaults _summonequipment)))
  (Variables|Default|SetSummonEquiped _newequip)
  (Utilities|Map|Add (Variables|/Game/DATA/Blueprints/Actors/BP_MasterItem.BP_MasterItem_C|GetVisualStatsBuff (Variables|Default|GetSummonEquiped)) "NewEnumerator8" (Math|Conversions|ToFloat(Integer) (.Mana%20Cost (Default|GetSkillStats (Variables|Default|GetStats%20Component) (Variables|Default|GetSkill)))))
  (Default|EquipedBuffStats (Variables|Default|GetSummonEquiped)))