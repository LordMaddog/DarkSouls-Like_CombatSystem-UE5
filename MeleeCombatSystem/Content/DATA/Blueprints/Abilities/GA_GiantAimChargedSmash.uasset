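; Giant aimed charged smash ability actor that performs a motion-warped dash attack toward the character's current target.
; DashAttack sets the attacking state, then, given a valid target, a short-delay loop keeps moving the "DashAttack" warp point to just short of that target.
; The first warp plays the main weapon's dash montage, or the combat component's fallback.
; Shortly before the montage ends, the ability levels the character's pitch and destroys itself.
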(event Custom|Update
  (Utilities|FlowControl|Delay 0.01)
  (if (Variables|Default|GetActive?)
    (CallFunction|SetDashActorTarget (Variables|/Game/DATA/Blueprints/Components/TargetingComponent.TargetingComponent_C|GetTarget%20Actor (Variables|/Game/DATA/BP_PC.BP_PC_C|GetTargetingComponent (Variables|Default|GetCharacter))) -2.7e+02)
    (CallFunction|Update)
    (CallFunction|Warp)))

(event Custom|Warp
  (Class|MotionWarpingComponent|AddorUpdateWarpTarget (Variables|Default|GetMotionWarping) (Utilities|Struct|MakeMotionWarpingTarget "DashAttack" (Variables|Default|GetL_DashToPoint) (Transformation|GetActorRotation (Variables|Default|GetCharacter)) 0 "None" false))
  (Utilities|FlowControl|DoOnce false
    (:Completed
      (Default|SetCurrentAction (Variables|Default|GetCombat%20Component) "(TagName=\"Character.Action.Attack.DashAttack\")")
      (bind _returnvalue (Animation|Montage|MontagePlay (Components|SkeletalMesh|GetAnimInstance (Variables|/Script/Engine.Character|GetMesh (Variables|Default|GetCharacter))) (select (Utilities|IsValid (Default|GetMainWeapon (Variables|Default|GetCombat%20Component))) (Utilities|Array|Get(acopy) (Variables|/Game/DATA/Blueprints/Actors/BP_BaseWeapon.BP_BaseWeapon_C|GetDashAttackMontages (Default|GetMainWeapon (Variables|Default|GetCombat%20Component))) (Variables|Default|GetIndex)) (Variables|/Game/DATA/Blueprints/Components/CombatComponent.CombatComponent_C|GetDashAttackAnim%20Montage (Variables|Default|GetCombat%20Component))) 1.0 "Duration" 0.0 true))
      (Utilities|FlowControl|Delay (- _returnvalue 1.5))
      (CallFunction|StopAbility))))

(event EventBeginPlay
  (|CallParentFunction) ; This node is disabled and will not be called.\nDrag off pins to build functionality.
)

(event EventStartAbility
  (|CallParentFunction)
  (Utilities|IsValid (Variables|/Game/DATA/Blueprints/Components/TargetingComponent.TargetingComponent_C|GetTarget%20Actor (Variables|/Game/DATA/BP_PC.BP_PC_C|GetTargetingComponent (Variables|Default|GetCharacter)))
    (:Is%20Valid
      (Variables|Default|SetActive? true)
      (CallFunction|SetDashActorTarget (Variables|/Game/DATA/Blueprints/Components/TargetingComponent.TargetingComponent_C|GetTarget%20Actor (Variables|/Game/DATA/BP_PC.BP_PC_C|GetTargetingComponent (Variables|Default|GetCharacter))) -2.7e+02)
      (CallFunction|Update)
      (CallFunction|Warp))))

(event EventStopAbility
  (bind _character (Variables|Default|GetCharacter))
  (bind _returnvalue (Transformation|GetActorRotation _character))
  (|CallParentFunction)
  (Variables|Default|SetActive? false)
  (Variables|Default|SetSet? false)
  (Transformation|SetActorRotation _character (Math|Rotator|MakeRotator (.roll _returnvalue) 0.0 (.yaw _returnvalue)) true)
  (Actor|DestroyActor))

(event EventDashAttack
  (params (DashRange :type Float%20%28double-precision%29))
  (Variables|Default|SetDistance DashRange)
  (Default|SetState (Variables|Default|GetCombat%20Component) "(TagName=\"Character.State.Attacking\")")
  (CallFunction|StartAbility))

(fn ConstructionScript
  (|CallParentFunction))

(fn SetDashActorTarget
  (params (InActor :type Actor%20Object%20Reference) (BackDistance :type Float%20%28single-precision%29))
  (Utilities|IsValid InActor
    (:Is%20Valid
      (Variables|Default|SetL_DashToPoint (+ (Transformation|GetActorLocation InActor) (* (Transformation|GetActorForwardVector (Variables|Default|GetCharacter)) BackDistance))))))