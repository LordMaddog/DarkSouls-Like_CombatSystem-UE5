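; Potion heal ability actor that restores a small random amount of health to its Character.
; On GAStart it applies point damage with a negated random value to the Character, so healing runs through the damage path as BP_AttackDamageType.
; The Character is also instigator and causer, and the ability actor destroys itself immediately afterward.
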(event EventBeginPlay
  (|CallParentFunction) ; This node is disabled and will not be called.\nDrag off pins to build functionality.
)

(event Collision|EventActorBeginOverlap
  (params (OtherActor :type Actor%20Object%20Reference)))

(event EventTick
  (params (DeltaSeconds :type Float%20%28single-precision%29)))

(event EventGAStart
  (bind _character (Variables|Default|GetCharacter))
  (bind _character_2 (Variables|Default|GetCharacter))
  (bind _returnvalue (Transformation|GetActorLocation _character_2))
  (Game|Damage|ApplyPointDamage _character_2 (* (Math|Random|RandomIntegerinRange 0 10) -1.0) _returnvalue (Collision|MakeHitResult false false 0.0 0.0 _returnvalue _returnvalue _returnvalue _returnvalue 0 (Variables|Default|GetCharacter)) (Pawn|GetController _character) _character "/Game/DATA/Blueprints/DamageTypes/BP_AttackDamageType.BP_AttackDamageType_C")
  (Actor|DestroyActor))

(fn ConstructionScript
  (|CallParentFunction))