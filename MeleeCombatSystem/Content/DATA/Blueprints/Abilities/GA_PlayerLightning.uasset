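; Player lightning ability actor that channels a lightning spell while the key is held.
; GAStart checks stamina, mana and combat state, then plays the attack montage; ActivateComboSkill spawns BP_lightningSpell at a hand socket, scaled by skill stats, and applies costs.
; HoldCheck re-polls input, montage, state and resources, calling Launch on failure to play the release montage and destroy the spell.
; Done uses a retriggerable delay as a timeout that removes the ability and cleans up.
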(event Custom|Launch
  ;[1 1 1] Launch the FireBall
  (if (Variables|Default|GetCharging)
    (Variables|Default|SetCharging false)
    (Default|PerformComboAction (Variables|Default|GetCombat%20Component) false (Variables|Default|GetAttackMontages2))
    (Actor|DestroyActor (Variables|Default|GetSpell))))

(event Custom|HoldCheck
  (bind _stats_component (Variables|Default|GetStats%20Component))
  (bind _skill (Variables|Default|GetSkill))
  (bind _stats_component_2 (Variables|Default|GetStats%20Component))
  (bind (_mana_cost _stamina_cost) (Default|GetSkillStats _stats_component _skill))
  ;[1 1 1] If key pressed and can still channle check.
  (if (Math|Boolean|ANDBoolean (== (Animation|Montage|GetCurrentActiveMontage (Components|SkeletalMesh|GetAnimInstance (Variables|/Script/Engine.Character|GetMesh (Variables|Default|GetCharacter)))) (Utilities|Array|Get(acopy) (Variables|Default|GetAttackMontages))) (Default|GetCurrentStateNotEqualAny (Variables|Default|GetCombat%20Component) "(GameplayTags=((TagName=\"Character.Action.Skill/Magic.Jump\"),(TagName=\"Character.State.Dodging\"),(TagName=\"Character.Action.Stuned\"),(TagName=\"Character.State.Attacking\"),(TagName=\"Character.State.Dead\"),(TagName=\"Character.State.Disabled\")))") (CallFunction|Hold?))
    (if (and (Default|StatGreaterThen _stats_component_2 "NewEnumerator4" (Math|Conversions|ToFloat(Integer) _mana_cost)) (Default|StatGreaterThen _stats_component_2 "NewEnumerator2" (Math|Conversions|ToFloat(Integer) _stamina_cost)))
      (Utilities|FlowControl|Delay 0.1)
      (CallFunction|HoldCheck)
      (CallFunction|Done 5.0)
      (Utilities|FlowControl|Delay 1.0)
      (Default|SetCurrentAction (Variables|Default|GetCombat%20Component) (Variables|Default|GetSkill))
      (else
        (Default|OOMCheck (Variables|Default|GetStats%20Component) 3.0)
        (CallFunction|Launch)))
    (else
      (CallFunction|Launch))))

(event EventBeginPlay
  (|CallParentFunction) ; This node is disabled and will not be called.\nDrag off pins to build functionality.
)

(event EventGAStart
  (bind _stats_component (Variables|Default|GetStats%20Component))
  (bind _stats_component_2 (Variables|Default|GetStats%20Component))
  (bind _skill (Variables|Default|GetSkill))
  (bind (_mana_cost _stamina_cost) (Default|GetSkillStats _stats_component_2 _skill))
  ;[1 1 1] Start
  (if (Math|Boolean|ANDBoolean (Default|StatGreaterThen _stats_component "NewEnumerator2" (Math|Conversions|ToFloat(Integer) _stamina_cost)) (Default|StatGreaterThen _stats_component "NewEnumerator4" (Math|Conversions|ToFloat(Integer) _mana_cost)) (Default|CanProformCombat (Variables|Default|GetCombat%20Component)))
    (Default|RotatetoTarget (Variables|Default|GetCharacter))
    (Variables|Default|SetCurrentPower 0.0)
    (Variables|Default|SetChargePower 0.0)
    (Default|PerformComboAction (Variables|Default|GetCombat%20Component) false (Variables|Default|GetAttackMontages))
    (Default|SetState (Variables|Default|GetCombat%20Component) "(TagName=\"Character.State.GenralActionState\")")
    (Variables|Default|SetCharging true)
    (CallFunction|Done 5.0)
    (else
      (Default|OOMCheck (Variables|Default|GetStats%20Component) (Math|Conversions|ToFloat(Integer) (.Stamina%20Cost (Default|GetSkillStats (Variables|Default|GetStats%20Component) (Variables|Default|GetSkill)))))
      (CallFunction|Done 5.0))))

(event EventActivateComboSkill
  (params (Hand :type E_Handed%20Enum :default "NewEnumerator0"))
  (bind _character (Variables|Default|GetCharacter))
  (bind _stats_component (Variables|Default|GetStats%20Component))
  (bind _stats_component_2 (Variables|Default|GetStats%20Component))
  (bind _skill (Variables|Default|GetSkill))
  (bind _skill_2 (Variables|Default|GetSkill))
  (bind (_mana_cost _stamina_cost _skill_xp _level_up_cost _skill_xpspent _skill_level _available_points _power _effectiveness) (Default|GetSkillStats _stats_component_2 _skill))
  (bind (_mana_cost_2 _stamina_cost_2) (Default|GetSkillStats _stats_component _skill_2))
  ;[1 1 1] Spawn
  (if (CallFunction|IsGAActive)
    (CallFunction|FloatWeapon true "NewEnumerator2" "NewEnumerator3")
    (bind _returnvalue (Game|SpawnActorfromClass "/Game/DATA/Blueprints/Actors/Magic/BP_lightningSpell.BP_lightningSpell_C" (Math|Transform|MakeTransform (Transformation|GetSocketLocation (Variables|/Script/Engine.Character|GetMesh (Variables|Default|GetCharacter)) "RHFS") "0, 0, 0" "1.000000,1.000000,1.000000") "Undefined" "MultiplyWithRoot" _character _power (* (* _power (Default|GetSubStats (Variables|Default|GetStats%20Component) "NewEnumerator12")) _effectiveness) (* 2e+03 _effectiveness) 0.0 _character _effectiveness false (Variables|Default|GetSkill) false 0.0 _character))
    (Variables|Default|SetSpell _returnvalue)
    (Default|SetActionCost (Variables|Default|GetStats%20Component) (Variables|Default|GetSkill) (Math|Conversions|ToFloat(Integer) _stamina_cost_2) (Math|Conversions|ToFloat(Integer) _mana_cost_2))
    (CallFunction|HoldCheck)))

(event EventDone
  (params (Duration :type Float%20%28single-precision%29))
  (bind _spell (Variables|Default|GetSpell))
  ;[1 1 1] End GA
  (Utilities|FlowControl|RetriggerableDelay Duration)
  (CallFunction|FloatWeapon false "NewEnumerator2" "NewEnumerator3")
  (Default|RemoveGA (Variables|/Game/DATA/BP_PC.BP_PC_C|GetCombatComponent (Variables|Default|GetCharacter)) (Utilities|GetClass self))
  (Utilities|IsValid _spell
    (:Is%20Valid
      (Actor|DestroyActor _spell))
    (:Is%20Not%20Valid
      _))
  (Actor|DestroyActor))

(fn ConstructionScript
  (|CallParentFunction))

(fn Hold?
  (return (and (Utilities|Enum|Equal(Enum) (Default|GetKeyStates (Variables|Default|GetCharacter) (Variables|Default|GetKeyIndex)) "NewEnumerator1") (Default|GetCurrentStateNotEqualAny (Variables|Default|GetCombat%20Component) "(GameplayTags=((TagName=\"Character.Action.Skill/Magic.Jump\"),(TagName=\"Character.State.Dodging\"),(TagName=\"Character.Action.Stuned\"),(TagName=\"Character.State.Attacking\"),(TagName=\"Character.State.Dead\"),(TagName=\"Character.State.Disabled\")))"))))