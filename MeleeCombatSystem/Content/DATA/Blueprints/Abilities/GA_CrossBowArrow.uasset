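; Actor-based crossbow ability for players and NPCs that reloads an unloaded crossbow or fires a loaded one, given equipped arrows.
; ActivateComboSkill spawns a bolt on the notch socket, and a looping timer aligns it and charges skill cost until loaded.
; An anim notify triggers the shot, launching the bolt along an aim trace with arrow-based gravity and consuming player ammo.
; NPCs re-trigger after loading, and a retriggerable delay removes the ability.
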(event Custom|ContinueCharge
  (bind _notchedarrow (CallFunction|GetNotchedArrow))
  (bind _cross_bow (Variables|Default|GetCross%20Bow))
  (bind _mainprojectilecore (Variables|/Game/DATA/Blueprints/Actors/BP_BaseSpell.BP_BaseSpell_C|GetMainProjectileCore _notchedarrow))
  (bind _itemskeletalmesh (Variables|/Game/DATA/Blueprints/Actors/BP_MasterItem.BP_MasterItem_C|GetItemSkeletalMesh _cross_bow))
  ;[1 1 1] Contuinue
  (Utilities|IsValid (Variables|Default|GetCharacter)
    (:Is%20Valid
      (CallFunction|Done 5.0)
      (Variables|Default|SetDrawling true)
      (Transformation|SetWorldRotation (Variables|/Game/DATA/Blueprints/Actors/BP_BaseSpell.BP_BaseSpell_C|GetMainProjectileCore (.NotchedArrow (CallFunction|GetNotchedArrow))) (Math|Rotator|FindLookatRotation (Transformation|GetSocketLocation _itemskeletalmesh "NotchSocket") (Transformation|GetSocketLocation _itemskeletalmesh "TipSocket")) false false)
      (CallFunction|ChargeCost)
      (if (Variables|/Game/DATA/Blueprints/Actors/Weapons/BP_BaseCrossBow.BP_BaseCrossBow_C|GetLoaded (Variables|Default|GetCross%20Bow))
        (Utilities|Time|ClearandInvalidateTimerbyHandle (Variables|Default|GetTimer))
        (Transformation|SetWorldLocation (Variables|/Game/DATA/Blueprints/Actors/BP_BaseSpell.BP_BaseSpell_C|GetMainProjectileCore (.NotchedArrow (CallFunction|GetNotchedArrow))) (+ (Transformation|GetWorldLocation _mainprojectilecore) (* (Math|Vector|GetRightVector _mainprojectilecore) 2.0)) false false)
        (Transformation|SetWorldRotation (Variables|/Game/DATA/Blueprints/Actors/BP_BaseSpell.BP_BaseSpell_C|GetMainProjectileCore (.NotchedArrow (CallFunction|GetNotchedArrow))) (Math|Rotator|FindLookatRotation (Transformation|GetWorldLocation (Variables|/Game/DATA/Blueprints/Actors/BP_BaseSpell.BP_BaseSpell_C|GetMainProjectileCore (.NotchedArrow (CallFunction|GetNotchedArrow)))) (Transformation|GetSocketLocation (Variables|/Game/DATA/Blueprints/Actors/BP_MasterItem.BP_MasterItem_C|GetItemSkeletalMesh (Variables|Default|GetCross%20Bow)) "TipSocket")) false false)
        (Animation|Montage|MontageSetPlayRate (Components|SkeletalMesh|GetAnimInstance (Variables|/Script/Engine.Character|GetMesh (Variables|Default|GetCharacter))) (Utilities|Array|Get(acopy) (Variables|/Game/DATA/Blueprints/Actors/BP_BaseWeapon.BP_BaseWeapon_C|GetLightAttackMontages (Variables|Default|GetCross%20Bow))) 1.0)
        (Variables|Default|SetDrawling false)
        (if (not (Variables|/Game/DATA/Blueprints/Components/CombatComponent.CombatComponent_C|GetIsPlayer (Variables|Default|GetCombat%20Component)))
          (Utilities|FlowControl|Delay (Math|Random|RandomFloatinRange 0.5 2.0))
          (Class|GamePlayAbilitiesBPI|GAStart(Message) self))))
    (:Is%20Not%20Valid
      (Actor|DestroyActor))))

(event Custom|ChargeCost
  (bind _skill (Variables|Default|GetSkill))
  (bind (_stamina _mana) (CallFunction|CheckManaStamina _skill))
  ;[1 1 1] Contuinue
  (Utilities|FlowControl|Delay 0.5)
  (if (and _stamina _mana)
    (if (Variables|/Game/DATA/Blueprints/Components/CombatComponent.CombatComponent_C|GetIsPlayer (Variables|Default|GetCombat%20Component))
      (Default|EventCost (Variables|Default|GetStats%20Component) (Variables|Default|GetSkill)))
    (else
      (Default|OOMCheck (Variables|Default|GetStats%20Component) (Math|Conversions|ToFloat(Integer) (.Stamina%20Cost (Default|GetSkillStats (Variables|Default|GetStats%20Component) _skill))))
      (Animation|Montage|MontageSetPlayRate (Components|SkeletalMesh|GetAnimInstance (Variables|/Script/Engine.Character|GetMesh (Variables|Default|GetCharacter))) (Utilities|Array|Get(acopy) (Variables|/Game/DATA/Blueprints/Actors/BP_BaseWeapon.BP_BaseWeapon_C|GetLightAttackMontages (Variables|Default|GetCross%20Bow))) 0.3))))

(event Custom|fired
  (bind _notchedarrow (CallFunction|GetNotchedArrow))
  (bind _notchedarrow_2 (CallFunction|GetNotchedArrow))
  (bind _cross_bow (Variables|Default|GetCross%20Bow))
  (bind _projectilemovement (Variables|/Game/DATA/Blueprints/Actors/BP_BaseSpell.BP_BaseSpell_C|GetProjectileMovement _notchedarrow_2))
  (bind _weaponmultiplierdamage (Variables|/Game/DATA/Blueprints/Actors/BP_BaseWeapon.BP_BaseWeapon_C|GetWeaponMultiplierDamage _cross_bow))
  (bind _returnvalue (* _weaponmultiplierdamage 3e+04))
  ;[1 1 1] Shoots off Arrow. (is called by anim notify)
  (Utilities|IsValid (.NotchedArrow (CallFunction|GetNotchedArrow))
    (:Is%20Valid
      (Transformation|DetachFromActor (.NotchedArrow (CallFunction|GetNotchedArrow)) "KeepWorld" "KeepWorld" "KeepWorld")
      (CallFunction|PlayBowSwingandArrowSound)
      (Components|Activation|Activate (Variables|/Game/DATA/Blueprints/Actors/BP_BaseSpell.BP_BaseSpell_C|GetProjectileMovement (.NotchedArrow (CallFunction|GetNotchedArrow))) true)
      (Utilities|FlowControl|Delay 0.01)
      (bind _returnvalue_2 (Default|GetAimTrace (Variables|Default|GetCombat%20Component) (Variables|/Game/DATA/BP_PC.BP_PC_C|GetFollowCamera (Variables|Default|GetCharacter)) (Variables|/Game/DATA/Blueprints/Actors/BP_BaseSpell.BP_BaseSpell_C|GetVisualEffect _notchedarrow) 6e+03 2e+01 (Variables|/Game/DATA/Blueprints/Components/CombatComponent.CombatComponent_C|GetDraw%20Debug%20Type (Variables|Default|GetCombat%20Component)) false "LHFS" _notchedarrow))
      (Transformation|SetActorRotation _notchedarrow_2 (select (Variables|/Game/DATA/Blueprints/Components/CombatComponent.CombatComponent_C|GetIsPlayer (Variables|Default|GetCombat%20Component)) (.rotation _returnvalue_2) (Math|Rotator|MakeRotator (.Roll (Math|Rotator|BreakRotator (.rotation _returnvalue_2))) (+ (.Pitch (Math|Rotator|BreakRotator (.rotation _returnvalue_2))) 1.5) (.Yaw (Math|Rotator|BreakRotator (.rotation _returnvalue_2))))))
      (Game|Components|ProjectileMovement|SetVelocityinLocalSpace _projectilemovement (Math|Vector|MakeVector (Math|Float|Clamp(Float) _returnvalue 5e+02 _returnvalue) 0.0 0.0))
      (Variables|/Script/Engine.ProjectileMovementComponent|SetProjectileGravityScale _projectilemovement (CallFunction|GetArrowsWeight))
      (CallFunction|Done 5.0)
      (CallFunction|SetNotLoaded)
      (CallFunction|Reset)
      (Collision|SetCollisionEnabled (Variables|/Game/DATA/Blueprints/Actors/BP_BaseSpell.BP_BaseSpell_C|GetMainProjectileCore (.NotchedArrow (CallFunction|GetNotchedArrow))) "QueryAndPhysics")
      (Variables|/Game/DATA/Blueprints/Actors/Weapons/BP_BaseCrossBow.BP_BaseCrossBow_C|SetNotchedArrow (Variables|Default|GetCross%20Bow) 0)
      (CallFunction|RemoveArrow)
      (Actor|Tick|SetActorTickEnabled false))
    (:Is%20Not%20Valid
      (CallFunction|SetNotLoaded)
      (CallFunction|Done 5.0))))

(event Custom|Reset
  (bind (_value _equipedarrows) (CallFunction|IsThereAnyArrows))
  (bind _timer (Variables|Default|GetTimer))
  (bind _character (Variables|Default|GetCharacter))
  (bind _combatcomponent (Variables|/Game/DATA/BP_PC.BP_PC_C|GetCombatComponent _character))
  ;[1 1 1] Start
  (Utilities|FlowControl|DoOnce false) ; enters at Reset
)

(event EventBeginPlay
  (|CallParentFunction) ; This node is disabled and will not be called.\nDrag off pins to build functionality.
)

(event Collision|EventActorBeginOverlap
  (params (OtherActor :type Actor%20Object%20Reference)))

(event EventGAStart
  (bind (_value _equipedarrows) (CallFunction|IsThereAnyArrows))
  (bind _timer (Variables|Default|GetTimer))
  (bind _character (Variables|Default|GetCharacter))
  (bind _combatcomponent (Variables|/Game/DATA/BP_PC.BP_PC_C|GetCombatComponent _character))
  ;[1 1 1] Start
  (if (Variables|/Game/DATA/Blueprints/Components/CombatComponent.CombatComponent_C|GetIsPlayer (Variables|Default|GetCombat%20Component))
    _
    (else
      (Utilities|FlowControl|Delay 0.1)
      (CallFunction|NPCGiveSkillifNoneExist "/Game/DATA/Blueprints/Actors/Useables/BP_ArcherySkillItem.BP_ArcherySkillItem_C" (Variables|Default|GetSkill))))
  (Utilities|FlowControl|DoOnce false
    (:Completed
      (if (not (Variables|Default|GetDrawling))
        (CallFunction|GetCrossBow :!label _label)
        (if (Default|CanProformCombat (Variables|Default|GetCombat%20Component))
          (if (Default|GetCombatEnabled _combatcomponent)
            (if _value
              (Variables|Default|SetEquiped%20Arrows _equipedarrows)
              (Default|RotatetoTarget (Variables|Default|GetCharacter))
              (if (Variables|/Game/DATA/Blueprints/Actors/Weapons/BP_BaseCrossBow.BP_BaseCrossBow_C|GetLoaded (Variables|Default|GetCross%20Bow))
                (Default|SetState (Variables|Default|GetCombat%20Component) "(TagName=\"Character.State.GenralActionState\")")
                (CallFunction|FireAnimation 0.0)
                (else
                  (CallFunction|SetCost)
                  (CallFunction|LoadAnimation (select (Variables|/Game/DATA/Blueprints/Components/CombatComponent.CombatComponent_C|GetIsPlayer (Variables|Default|GetCombat%20Component)) (- (.Power (Default|GetSkillStats (Variables|Default|GetStats%20Component) (Variables|Default|GetSkill))) 0.6) (Math|Random|RandomFloatinRange 1.0 2.0)))
                  (Default|SetState (Variables|Default|GetCombat%20Component) "(TagName=\"Character.State.GenralActionState\")")
                  (CallFunction|Reset)))
              (else
                (CallFunction|Done 5.0 :!label _label_2)
                (CallFunction|Reset)))
            (else
              (Default|Draw/sheathWeapon _combatcomponent)
              (goto _label_2)))
          (else
            (goto _label_2)))
        (elif (== (Animation|Montage|GetCurrentActiveMontage (Components|SkeletalMesh|GetAnimInstance (Variables|/Script/Engine.Character|GetMesh (Variables|Default|GetCharacter)))) "/Game/DATA/Animations/CrossBow/CrossBow_Reload_Montage.CrossBow_Reload_Montage")
          (CallFunction|Reset)
          (else
            (if (Utilities|Time|IsValidTimerHandle _timer)
              (Utilities|Time|ClearandInvalidateTimerbyHandle _timer))
            (Variables|Default|SetDrawling false)
            (goto _label)))))))

(event EventActivateComboSkill
  (params (Hand :type E_Handed%20Enum :default "NewEnumerator0"))
  (bind _character (Variables|Default|GetCharacter))
  (bind _cross_bow (Variables|Default|GetCross%20Bow))
  (bind _cross_bow_2 (Variables|Default|GetCross%20Bow))
  (bind _itemskeletalmesh (Variables|/Game/DATA/Blueprints/Actors/BP_MasterItem.BP_MasterItem_C|GetItemSkeletalMesh _cross_bow_2))
  ;[1 1 1] Spawn
  (if (not (Variables|/Game/DATA/Blueprints/Actors/Weapons/BP_BaseCrossBow.BP_BaseCrossBow_C|GetLoaded (Variables|Default|GetCross%20Bow)))
    (CallFunction|Done 5.0)
    (Default|SetState (Variables|Default|GetCombat%20Component) "(TagName=\"Character.State.GenralActionState\")")
    (bind _returnvalue (Game|SpawnActorfromClass "/Game/DATA/Blueprints/Actors/Magic/BP_BaseArrowSpell.BP_BaseArrowSpell_C" (Math|Transform|MakeTransform (Transformation|GetSocketLocation (Variables|/Game/DATA/Blueprints/Actors/BP_MasterItem.BP_MasterItem_C|GetItemSkeletalMesh (Variables|Default|GetCross%20Bow)) "NotchSocket") (Math|Rotator|FindLookatRotation (Transformation|GetSocketLocation _itemskeletalmesh "NotchSocket") (Transformation|GetSocketLocation _itemskeletalmesh "TipSocket")) "1.000000,1.000000,1.000000") "Undefined" "MultiplyWithRoot" _character (Variables|/Game/DATA/Blueprints/Actors/BP_BaseWeapon.BP_BaseWeapon_C|GetWeaponMultiplierDamage _cross_bow) 1e+01 2e+04 0.0 _character (- (+ (Variables|/Game/DATA/Blueprints/Actors/BP_BaseWeapon.BP_BaseWeapon_C|GetBasePoiseDamgeMultiplier _cross_bow) (.Effectiveness (Default|GetSkillStats (Variables|Default|GetStats%20Component) (Variables|Default|GetSkill)))) 1.0) true "(TagName=\"Character.Action.Skill/Magic.Archery\")" false 0.0 _character))
    (bind _output_get (CallFunction|SetNotchedArrow _returnvalue))
    (Transformation|AttachComponentToComponent _output_get (Variables|/Game/DATA/Blueprints/Actors/BP_MasterItem.BP_MasterItem_C|GetItemSkeletalMesh (Variables|Default|GetCross%20Bow)) "NotchSocket" "KeepWorld" "KeepWorld" "KeepWorld" true)
    (bind (_class _value) (CallFunction|GetArrowType))
    (if _value
      (CallFunction|ChangeVisualArrow _class))
    (if (Utilities|Time|IsValidTimerHandle (Variables|Default|GetTimer))
      (Utilities|Time|ClearandInvalidateTimerbyHandle (Variables|Default|GetTimer)))
    (bind _returnvalue_2 (Utilities|Time|SetTimerbyFunctionName 0 "ContinueCharge" 0.01 true))
    (Variables|Default|SetTimer _returnvalue_2)
    (CallFunction|ContinueCharge)
    (else
      (CallFunction|Fired))))

(event EventGAStop
  (bind _notchedarrow (CallFunction|GetNotchedArrow))
  (bind _notchedarrow_2 (CallFunction|GetNotchedArrow))
  (bind _cross_bow (Variables|Default|GetCross%20Bow))
  (bind _projectilemovement (Variables|/Game/DATA/Blueprints/Actors/BP_BaseSpell.BP_BaseSpell_C|GetProjectileMovement _notchedarrow_2))
  (bind _weaponmultiplierdamage (Variables|/Game/DATA/Blueprints/Actors/BP_BaseWeapon.BP_BaseWeapon_C|GetWeaponMultiplierDamage _cross_bow))
  (bind _returnvalue (* _weaponmultiplierdamage 3e+04))
  ;[1 1 1] Shoots off Arrow. (is called by anim notify)
  (Utilities|IsValid (.NotchedArrow (CallFunction|GetNotchedArrow))
    (:Is%20Valid
      (Transformation|DetachFromActor (.NotchedArrow (CallFunction|GetNotchedArrow)) "KeepWorld" "KeepWorld" "KeepWorld")
      (CallFunction|PlayBowSwingandArrowSound)
      (Components|Activation|Activate (Variables|/Game/DATA/Blueprints/Actors/BP_BaseSpell.BP_BaseSpell_C|GetProjectileMovement (.NotchedArrow (CallFunction|GetNotchedArrow))) true)
      (Utilities|FlowControl|Delay 0.01)
      (bind _returnvalue_2 (Default|GetAimTrace (Variables|Default|GetCombat%20Component) (Variables|/Game/DATA/BP_PC.BP_PC_C|GetFollowCamera (Variables|Default|GetCharacter)) (Variables|/Game/DATA/Blueprints/Actors/BP_BaseSpell.BP_BaseSpell_C|GetVisualEffect _notchedarrow) 6e+03 2e+01 (Variables|/Game/DATA/Blueprints/Components/CombatComponent.CombatComponent_C|GetDraw%20Debug%20Type (Variables|Default|GetCombat%20Component)) false "LHFS" _notchedarrow))
      (Transformation|SetActorRotation _notchedarrow_2 (select (Variables|/Game/DATA/Blueprints/Components/CombatComponent.CombatComponent_C|GetIsPlayer (Variables|Default|GetCombat%20Component)) (.rotation _returnvalue_2) (Math|Rotator|MakeRotator (.Roll (Math|Rotator|BreakRotator (.rotation _returnvalue_2))) (+ (.Pitch (Math|Rotator|BreakRotator (.rotation _returnvalue_2))) 1.5) (.Yaw (Math|Rotator|BreakRotator (.rotation _returnvalue_2))))))
      (Game|Components|ProjectileMovement|SetVelocityinLocalSpace _projectilemovement (Math|Vector|MakeVector (Math|Float|Clamp(Float) _returnvalue 5e+02 _returnvalue) 0.0 0.0))
      (Variables|/Script/Engine.ProjectileMovementComponent|SetProjectileGravityScale _projectilemovement (CallFunction|GetArrowsWeight))
      (CallFunction|Done 5.0)
      (CallFunction|SetNotLoaded)
      (CallFunction|Reset)
      (Collision|SetCollisionEnabled (Variables|/Game/DATA/Blueprints/Actors/BP_BaseSpell.BP_BaseSpell_C|GetMainProjectileCore (.NotchedArrow (CallFunction|GetNotchedArrow))) "QueryAndPhysics")
      (Variables|/Game/DATA/Blueprints/Actors/Weapons/BP_BaseCrossBow.BP_BaseCrossBow_C|SetNotchedArrow (Variables|Default|GetCross%20Bow) 0)
      (CallFunction|RemoveArrow)
      (Actor|Tick|SetActorTickEnabled false))
    (:Is%20Not%20Valid
      (CallFunction|SetNotLoaded)
      (CallFunction|Done 5.0))))

(event EventDone
  (params (Duration :type Float%20%28single-precision%29))
  ;[1 1 1] End GA
  (Utilities|FlowControl|RetriggerableDelay Duration)
  (Utilities|IsValid (Variables|Default|GetCharacter)
    (:Is%20Valid
      (CallFunction|FloatWeapon false "NewEnumerator2" "NewEnumerator2")
      (Default|RemoveGA (Variables|/Game/DATA/BP_PC.BP_PC_C|GetCombatComponent (Variables|Default|GetCharacter)) (Utilities|GetClass self))
      (Actor|DestroyActor))))

(event EventTick
  (params (DeltaSeconds :type Float%20%28single-precision%29))
  ;[1 1 1] Spawn
  (Utilities|IsValid (Variables|Default|GetCharacter)
    (:Is%20Valid
      (Default|RotatetoCamera (Variables|Default|GetTargetingComponent) 8.0))
    (:Is%20Not%20Valid
      (Actor|DestroyActor))))

(fn ConstructionScript
  (|CallParentFunction))

(fn SetCost
  (bind _skill (Variables|Default|GetSkill))
  (bind _stats_component (Variables|Default|GetStats%20Component))
  (bind (_combat_types _mana_cost _stamina_cost) (Default|GetSkillStats _stats_component _skill))
  (Default|SetActionCost (Variables|Default|GetStats%20Component) (Variables|Default|GetSkill) (Math|Conversions|ToFloat(Integer) (Math|Integer|Clamp(Integer) _stamina_cost 1 _stamina_cost)) (Math|Conversions|ToFloat(Integer) (Math|Integer|Clamp(Integer) _mana_cost 0 _mana_cost))))

(fn PlayBowSwingandArrowSound
  (Components|Activation|Activate (Variables|/Game/DATA/Blueprints/Actors/Weapons/BP_BaseCrossBow.BP_BaseCrossBow_C|GetCrossBowFire (Variables|Default|GetCross%20Bow)) true)
  (Components|Activation|Activate (Variables|/Game/DATA/Blueprints/Actors/BP_BaseSpell.BP_BaseSpell_C|GetFlySound (.NotchedArrow (CallFunction|GetNotchedArrow))) true)
  (Components|Activation|Activate (Variables|/Game/DATA/Blueprints/Actors/BP_BaseSpell.BP_BaseSpell_C|GetTrail (.NotchedArrow (CallFunction|GetNotchedArrow))) true))

(fn IsThereAnyArrows
  (bind _keys (Utilities|Map|Keys (Variables|/Game/DATA/Blueprints/Components/EquipmentComponet.EquipmentComponet_C|GetEquiped (Variables|/Game/DATA/BP_PC.BP_PC_C|GetEquipmentComponet (Variables|Default|GetCharacter)))))
  (for _array_element _keys
    (if (Utilities|Enum|Equal(Enum) (.EquipType (Utilities|Struct|BreakS_EquippedItemInfo (.Value (Utilities|Map|Find (Variables|/Game/DATA/Blueprints/Components/EquipmentComponet.EquipmentComponet_C|GetEquiped (Variables|/Game/DATA/BP_PC.BP_PC_C|GetEquipmentComponet (Variables|Default|GetCharacter))) _array_element)))) "NewEnumerator29")
      (return true (.EquipedItem (Utilities|Struct|BreakS_EquippedItemInfo (.Value (Utilities|Map|Find (Variables|/Game/DATA/Blueprints/Components/EquipmentComponet.EquipmentComponet_C|GetEquiped (Variables|/Game/DATA/BP_PC.BP_PC_C|GetEquipmentComponet (Variables|Default|GetCharacter))) _array_element)))))))
  (return false 0))

(fn RemoveArrow
  (bind _character (Variables|Default|GetCharacter))
  (bind _character_2 (Variables|Default|GetCharacter))
  (bind _inventory (Variables|/Game/DATA/BP_PC.BP_PC_C|GetInventory _character))
  (bind _inventory_2 (Variables|/Game/DATA/BP_PC.BP_PC_C|GetInventory _character_2))
  (bind _mainwidget (Variables|/Game/DATA/Blueprints/Actors/Inventory/BP_Inventory.BP_Inventory_C|GetMainWidget _inventory_2))
  (bind _arrowslots (Variables|/Game/DATA/Blueprints/Actors/Inventory/BP_Inventory.BP_Inventory_C|GetArrowSlots _inventory))
  (bind _cw_equipmentwidget (Variables|/Game/DATA/UI/Inventory/WBP_MainWidget.WBP_MainWidget_C|GetCW_EquipmentWidget _mainwidget))
  (bind _cw_arrows (Variables|/Game/DATA/UI/Inventory/CW_EquipmentWidget.CW_EquipmentWidget_C|GetCW_Arrows _cw_equipmentwidget))
  (if (Variables|/Game/DATA/Blueprints/Components/CombatComponent.CombatComponent_C|GetIsPlayer (Variables|Default|GetCombat%20Component))
    (Default|RemoveItematIndexAlt _inventory 0 1 false _arrowslots)
    (if (Default|IsSlotEmptyAlt _inventory 0 _arrowslots)
      (Utilities|IsValid _cw_arrows
        (:Is%20Valid
          (Default|UnequipItem _cw_arrows false)
          (return)))
      (else
        (return)))
    (else
      (return))))

(fn GetArrowType
  (bind _keys (Utilities|Map|Keys (Variables|/Game/DATA/Blueprints/Components/EquipmentComponet.EquipmentComponet_C|GetEquiped (Variables|/Game/DATA/BP_PC.BP_PC_C|GetEquipmentComponet (Variables|Default|GetCharacter)))))
  (for _array_element _keys
    (if (Utilities|Enum|Equal(Enum) (.EquipType (Utilities|Struct|BreakS_EquippedItemInfo (.Value (Utilities|Map|Find (Variables|/Game/DATA/Blueprints/Components/EquipmentComponet.EquipmentComponet_C|GetEquiped (Variables|/Game/DATA/BP_PC.BP_PC_C|GetEquipmentComponet (Variables|Default|GetCharacter))) _array_element)))) "NewEnumerator29")
      (return _array_element true)))
  (return 0 false))

(fn ChangeVisualArrow
  (params (Item%20Class :type BP%20Master%20Item%20Class%20Reference))
  (bind _notchedarrow (CallFunction|GetNotchedArrow))
  (bind _output_get (Variables|/Game/DATA/Blueprints/Actors/Magic/BP_BaseArrowSpell.BP_BaseArrowSpell_C|SetItem%20Class _notchedarrow Item%20Class))
  (Components|StaticMesh|SetStaticMesh (Variables|/Game/DATA/Blueprints/Actors/BP_BaseSpell.BP_BaseSpell_C|GetVisualEffect _notchedarrow) (Utilities|GetClassDefaults _output_get)))

(fn GetArrowsWeight
  (bind _equiped_arrows (Variables|Default|GetEquiped%20Arrows))
  (bind _substatsbuff (Variables|/Game/DATA/Blueprints/Actors/BP_MasterItem.BP_MasterItem_C|GetSubStatsBuff _equiped_arrows))
  (bind (_value _returnvalue) (Utilities|Map|Find _substatsbuff "NewEnumerator32"))
  (return (select _returnvalue _value 1.0)))

(fn GetIntiCrossBow
  (bind _combat_component (Variables|Default|GetCombat%20Component))
  (bind _returnvalue (Default|GetMainWeapon _combat_component))
  (bind _equipedoffhand (Default|GetOffHandedWeapon _combat_component))
  (bind _twohandedcombattype (Variables|/Game/DATA/Blueprints/Actors/BP_BaseWeapon.BP_BaseWeapon_C|GetTwoHandedCombatType _returnvalue))
  (bind _returnvalue_2 (Utilities|Enum|Equal(Enum) _twohandedcombattype "NewEnumerator7"))
  (bind _returnvalue_3 (select _returnvalue_2 _returnvalue _equipedoffhand))
  (return (Variables|/Game/DATA/Blueprints/Actors/BP_MasterItem.BP_MasterItem_C|GetItemSkeletalMesh _returnvalue_3) _returnvalue_3))

(fn LoadAnimation
  (params (DrawSpeed :type Float%20%28double-precision%29))
  (bind _cross_bow (Variables|Default|GetCross%20Bow))
  (bind _crossbowdraw (Variables|/Game/DATA/Blueprints/Actors/Weapons/BP_BaseCrossBow.BP_BaseCrossBow_C|GetCrossBowDraw _cross_bow))
  (Animation|PlayAnimMontage (Variables|Default|GetCharacter) (Utilities|Array|Get(acopy) (Variables|/Game/DATA/Blueprints/Actors/BP_BaseWeapon.BP_BaseWeapon_C|GetLightAttackMontages (Variables|Default|GetCross%20Bow))) DrawSpeed "None")
  (Animation|Montage|MontagePlay (Components|SkeletalMesh|GetAnimInstance (Variables|/Game/DATA/Blueprints/Actors/BP_MasterItem.BP_MasterItem_C|GetItemSkeletalMesh (Variables|Default|GetCross%20Bow))) "/Game/DATA/Animations/CrossBow/CrossBowRigAnimations/CrossBowRigged_Reload_Montage.CrossBowRigged_Reload_Montage" DrawSpeed "MontageLength" 0.0 true)
  (Audio|Components|Audio|SetPitchMultiplier _crossbowdraw DrawSpeed)
  (Components|Activation|Activate _crossbowdraw true)
  (return))

(fn GetCrossBow
  (Variables|Default|GetCross%20Bow
    (:then
      _)
    (:else
      (bind _asbp_base_cross_bow (Utilities|Casting|CastToBP_BaseCrossBow (.ReturnValue (CallFunction|GetIntiCrossBow))))
      (Variables|Default|SetCross%20Bow _asbp_base_cross_bow)))
  (return))

(fn FireAnimation
  (params (DrawSpeed :type Float%20%28double-precision%29))
  (Animation|PlayAnimMontage (Variables|Default|GetCharacter) (Utilities|Array|Get(acopy) (Variables|/Game/DATA/Blueprints/Actors/BP_BaseWeapon.BP_BaseWeapon_C|GetLightAttackMontages (Variables|Default|GetCross%20Bow)) 1) 1.0 "None")
  (Animation|Montage|MontagePlay (Components|SkeletalMesh|GetAnimInstance (Variables|/Game/DATA/Blueprints/Actors/BP_MasterItem.BP_MasterItem_C|GetItemSkeletalMesh (Variables|Default|GetCross%20Bow))) "/Game/DATA/Animations/CrossBow/CrossBowRigAnimations/CrossBow_Fire_Montage.CrossBow_Fire_Montage" 0.5 "MontageLength" 0.0 true)
  (return))

(fn SetNotchedArrow
  (params (NotchedArrow :type BP%20Base%20Arrow%20Spell%20Object%20Reference))
  (Utilities|IsValid (Variables|/Game/DATA/Blueprints/Actors/Weapons/BP_BaseCrossBow.BP_BaseCrossBow_C|GetNotchedArrow (Variables|Default|GetCross%20Bow))
    (:Is%20Valid
      (Actor|DestroyActor (Variables|/Game/DATA/Blueprints/Actors/Weapons/BP_BaseCrossBow.BP_BaseCrossBow_C|GetNotchedArrow (Variables|Default|GetCross%20Bow))))
    (:Is%20Not%20Valid
      _))
  (bind _output_get (Variables|/Game/DATA/Blueprints/Actors/Weapons/BP_BaseCrossBow.BP_BaseCrossBow_C|SetNotchedArrow (Variables|Default|GetCross%20Bow) NotchedArrow))
  (Default|SetBolt _output_get)
  (return _output_get))

(fn GetNotchedArrow
  (bind _cross_bow (Variables|Default|GetCross%20Bow))
  (bind _notchedarrow (Variables|/Game/DATA/Blueprints/Actors/Weapons/BP_BaseCrossBow.BP_BaseCrossBow_C|GetNotchedArrow _cross_bow))
  (Utilities|IsValid _notchedarrow
    (:Is%20Valid
      (return _notchedarrow true))
    (:Is%20Not%20Valid
      (return 0 false))))

(fn SetNotLoaded
  (Class|AnimBPI|CrossBowLoaded(Message) (Components|SkeletalMesh|GetAnimInstance (Variables|/Game/DATA/Blueprints/Actors/BP_MasterItem.BP_MasterItem_C|GetItemSkeletalMesh (Variables|Default|GetCross%20Bow))) false)
  (Variables|/Game/DATA/Blueprints/Actors/Weapons/BP_BaseCrossBow.BP_BaseCrossBow_C|SetLoaded (Variables|Default|GetCross%20Bow) false))