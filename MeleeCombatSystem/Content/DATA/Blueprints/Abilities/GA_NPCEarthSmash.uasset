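; NPC ability actor for the Earth Smash magic skill, a montage-driven attack that spawns a ground effect.
; GAStart grants the skill, checks stamina, mana and combat state, then sets weapon damage, hyper armor, action cost and hand effects.
; ActivateComboSkill traces down ahead of the character and spawns BP_EarthSmash, scaled by skill and sub-stats.
; Done uses a retriggerable delay to undo the effects, destroying the actor if the weapon is valid.
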(event EventBeginPlay
  (|CallParentFunction) ; This node is disabled and will not be called.\nDrag off pins to build functionality.
)

(event Collision|EventActorBeginOverlap
  (params (OtherActor :type Actor%20Object%20Reference)))

(event EventTick
  (params (DeltaSeconds :type Float%20%28single-precision%29)))

(event EventGAStart
  (bind _stats_component (Variables|Default|GetStats%20Component))
  (bind _stats_component_2 (Variables|Default|GetStats%20Component))
  (bind _stats_component_3 (Variables|Default|GetStats%20Component))
  (bind _stats_component_4 (Variables|Default|GetStats%20Component))
  (bind (_mana_cost _stamina_cost) (Default|GetSkillStats _stats_component_4 "(TagName=\"Character.Action.Skill/Magic.EarthSmash\")"))
  (bind (_mana_cost_2 _stamina_cost_2) (Default|GetSkillStats _stats_component_2 "(TagName=\"Character.Action.Skill/Magic.EarthSmash\")"))
  (bind (_mana_cost_3 _stamina_cost_3 _skill_xp _level_up_cost _skill_xpspent _skill_level _available_points _power _effectiveness) (Default|GetSkillStats _stats_component_3 "(TagName=\"Character.Action.Skill/Magic.EarthSmash\")"))
  ;[1 1 1] Start
  (CallFunction|NPCGiveSkillifNoneExist "/Game/DATA/Blueprints/Actors/Useables/BP_EarthSmashItem.BP_EarthSmashItem_C" "(TagName=\"Character.Action.Skill/Magic.EarthSmash\")")
  (if (Math|Boolean|ANDBoolean (Default|StatGreaterThen _stats_component "NewEnumerator2" (Math|Conversions|ToFloat(Integer) _stamina_cost_2)) (Default|StatGreaterThen _stats_component "NewEnumerator4" (Math|Conversions|ToFloat(Integer) _mana_cost_2)) (Default|CanProformCombat (Variables|Default|GetCombat%20Component)))
    (Default|RotatetoTarget (Variables|Default|GetCharacter))
    (bind _output_get (Default|SetMeleeSkillUsed (Default|GetMainWeapon (Variables|/Game/DATA/BP_PC.BP_PC_C|GetCombatComponent (Variables|Default|GetCharacter))) "(TagName=\"Character.Action.Skill/Magic.EarthSmash\")"))
    (Default|SetActionDamageMultiplyer (Default|GetMainWeapon (Variables|/Game/DATA/BP_PC.BP_PC_C|GetCombatComponent (Variables|Default|GetCharacter))) _output_get _power _effectiveness)
    (CallFunction|EquipHyperArmor)
    (Default|PerformComboAction (Variables|Default|GetCombat%20Component) false (Variables|Default|GetAttackMontages))
    (Default|SetState (Variables|Default|GetCombat%20Component) "(TagName=\"Character.State.GenralActionState\")")
    (Default|SetActionCost (Variables|Default|GetStats%20Component) "(TagName=\"Character.Action.Skill/Magic.EarthSmash\")" (Math|Conversions|ToFloat(Integer) _stamina_cost) (Math|Conversions|ToFloat(Integer) _mana_cost))
    (Default|SetCurrentAction (Variables|Default|GetCombat%20Component) "(TagName=\"Character.Action.Skill/Magic.EarthSmash\")")
    (CallFunction|Done 4.0)
    (CallFunction|MagicHands "NewEnumerator2" "NewEnumerator1" true)
    (else
      (Default|OOMCheck (Variables|Default|GetStats%20Component) (Math|Conversions|ToFloat(Integer) (.Stamina%20Cost (Default|GetSkillStats (Variables|Default|GetStats%20Component) "(TagName=\"Character.Action.Skill/Magic.EarthSmash\")"))))
      (CallFunction|Done 4.0))))

(event EventActivateComboSkill
  (params (Hand :type E_Handed%20Enum :default "NewEnumerator0"))
  (bind _character (Variables|Default|GetCharacter))
  (bind _character_2 (Variables|Default|GetCharacter))
  (bind _stats_component (Variables|Default|GetStats%20Component))
  (bind _character_3 (Variables|Default|GetCharacter))
  (bind (_mana_cost _stamina_cost _skill_xp _level_up_cost _skill_xpspent _skill_level _available_points _power _effectiveness) (Default|GetSkillStats _stats_component "(TagName=\"Character.Action.Skill/Magic.EarthSmash\")"))
  (bind _returnvalue (Transformation|GetActorForwardVector _character_3))
  (bind _returnvalue_2 (Transformation|GetActorLocation _character_3))
  (bind _returnvalue_3 (* _returnvalue 1e+02))
  (bind _returnvalue_4 (+ _returnvalue_2 _returnvalue_3))
  ;[1 1 1] Spawn
  (bind (_outhit _returnvalue_5) (Collision|LineTraceByChannel _returnvalue_4 (- _returnvalue_4 "0.000000,0.000000,150.000000") "TraceTypeQuery1" false (Utilities|Array|MakeArray _character_2) (Variables|/Game/DATA/Blueprints/Components/CombatComponent.CombatComponent_C|GetDraw%20Debug%20Type (Variables|/Game/DATA/BP_PC.BP_PC_C|GetCombatComponent _character_2))))
  (if _returnvalue_5
    (Game|SpawnActorfromClass "/Game/DATA/Blueprints/Actors/Magic/BP_EarthSmash.BP_EarthSmash_C" (Math|Transform|MakeTransform (+ (.Location (Collision|BreakHitResult _outhit)) "0.000000,0.000000,10.000000") (Transformation|GetActorRotation (Variables|Default|GetCharacter)) (* 1.1 (+ _effectiveness (* (Default|GetSubStats (Variables|Default|GetStats%20Component) "NewEnumerator12") 0.02)))) "AlwaysSpawn" "MultiplyWithRoot" _character _power 157.441377 3.5e+02 1e+03 _character _effectiveness false "(TagName=\"Character.Action.Skill/Magic.EarthSmash\")" false 0.0 _character)))

(event EventDone
  (params (Duration :type Float%20%28single-precision%29))
  (bind _character (Variables|Default|GetCharacter))
  (bind _combatcomponent (Variables|/Game/DATA/BP_PC.BP_PC_C|GetCombatComponent _character))
  (bind _returnvalue (Default|GetMainWeapon _combatcomponent))
  ;[1 1 1] Done
  (Utilities|FlowControl|RetriggerableDelay Duration)
  (CallFunction|FloatWeapon false "NewEnumerator2" "NewEnumerator0")
  (CallFunction|MagicHands "NewEnumerator2" "NewEnumerator0" false)
  (CallFunction|UnEquipHyperArmor)
  (Utilities|IsValid _returnvalue
    (:Is%20Valid
      (Default|SetMeleeSkillUsed _returnvalue)
      (Actor|DestroyActor))))

(fn ConstructionScript
  (|CallParentFunction))