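; Actor-based ability that fires or reloads the character's gun, with leftover bow-and-arrow code that is mostly unwired.
; GAStart checks stamina, mana and combat state, draws a sheathed weapon or checks ammo, then loops the aim-up montage until targeting reports alignment while Tick rotates toward camera.
; ActivateComboSkill spawns BP_Bullet along an aim trace with gun effects, or refills ammo when reloading.
; A retriggerable delay removes and destroys the ability.
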(event Custom|Reload
  ;[1 1 1] Spawn
  (Variables|/Game/DATA/Blueprints/Actors/Weapons/BP_BaseGun.BP_BaseGun_C|SetAmmo (Variables|Default|GetGun) (Math|Float|Truncate (* (Default|GetCurrentStatValue (Variables|Default|GetStats%20Component) "NewEnumerator4") 0.5)))
  (Default|UpdateTex (Variables|Default|GetGun))
  (Default|SetCurrentStatValue (Variables|Default|GetStats%20Component) "NewEnumerator4" 1.0)
  (CallFunction|Reset)
  (Variables|Default|SetReLoading false))

(event Custom|IsAimed
  (params (Value :type Boolean))
  (Variables|Default|SetAimAligned Value))

(event Custom|Reset
  (bind _skill (Variables|Default|GetSkill))
  (bind _character (Variables|Default|GetCharacter))
  (bind (_stamina _mana) (CallFunction|CheckManaStamina _skill))
  (bind _combatcomponent (Variables|/Game/DATA/BP_PC.BP_PC_C|GetCombatComponent _character))
  ;[1 1 1] Start
  (Utilities|FlowControl|DoOnce false) ; enters at Reset
)

(event EventBeginPlay
  (bind _targetingcomponent (Variables|Default|GetTargetingComponent))
  (|CallParentFunction)
  (Utilities|IsValid _targetingcomponent
    (:Is%20Valid
      (EventDispatchers|BindEventtoAimed _targetingcomponent (delegate Custom|IsAimed)))))

(event Collision|EventActorBeginOverlap
  (params (OtherActor :type Actor%20Object%20Reference)))

(event EventGAStart
  (bind _skill (Variables|Default|GetSkill))
  (bind _character (Variables|Default|GetCharacter))
  (bind (_stamina _mana) (CallFunction|CheckManaStamina _skill))
  (bind _combatcomponent (Variables|/Game/DATA/BP_PC.BP_PC_C|GetCombatComponent _character))
  ;[1 1 1] Start
  (if (Variables|/Game/DATA/Blueprints/Components/CombatComponent.CombatComponent_C|GetIsPlayer (Variables|Default|GetCombat%20Component))
    _
    (else
      (Utilities|FlowControl|Delay 0.1)
      (CallFunction|NPCGiveSkillifNoneExist "/Game/DATA/Blueprints/Actors/Useables/BP_ArcherySkillItem.BP_ArcherySkillItem_C" (Variables|Default|GetSkill))))
  (Utilities|FlowControl|DoOnce false
    (:Completed
      (if (Math|Boolean|ANDBoolean _stamina _mana (Default|CanProformCombat (Variables|Default|GetCombat%20Component)))
        (if (Default|GetCombatEnabled _combatcomponent)
          (bind _returnvalue (CallFunction|GetAmmo))
          (if _returnvalue
            (Actor|Tick|SetActorTickEnabled true)
            (if (Variables|Default|GetAimAligned) :!label _label
              (CallFunction|FireAnimation)
              (Default|SetState (Variables|Default|GetCombat%20Component) "(TagName=\"Character.State.GenralActionState\")")
              (CallFunction|Done 5.0)
              (Variables|Default|SetTick%20Count 0.0)
              (else
                (CallFunction|AimUpAnimation)
                (Utilities|FlowControl|Delay 0.05)
                (goto _label)))
            (else
              (Variables|Default|SetReLoading true)
              (CallFunction|ReloadAnimation)
              (Default|SetState (Variables|Default|GetCombat%20Component) "(TagName=\"Character.State.GenralActionState\")")))
          (else
            (Default|Draw/sheathWeapon _combatcomponent)
            (CallFunction|Done 3.0)
            (CallFunction|Reset)))
        (else
          (Default|OOMCheck (Variables|Default|GetStats%20Component) (Math|Conversions|ToFloat(Integer) (.Stamina%20Cost (Default|GetSkillStats (Variables|Default|GetStats%20Component) (Variables|Default|GetSkill)))))
          (CallFunction|Done 5.0)
          (CallFunction|Reset))))))

(event EventActivateComboSkill
  (params (Hand :type E_Handed%20Enum :default "NewEnumerator0"))
  (bind _combat_component (Variables|Default|GetCombat%20Component))
  (bind _character (Variables|Default|GetCharacter))
  (bind _returnvalue (Default|GetMainWeapon _combat_component))
  ;[1 1 1] Spawn
  (if (not (Variables|Default|GetReLoading))
    (CallFunction|GunAnimation)
    (CallFunction|Done 5.0)
    (bind _returnvalue_2 (Default|GetAimTrace (Variables|Default|GetCombat%20Component) (Variables|/Game/DATA/BP_PC.BP_PC_C|GetFollowCamera (Variables|Default|GetCharacter)) (Variables|/Game/DATA/Blueprints/Actors/BP_MasterItem.BP_MasterItem_C|GetItemStaticMesh _returnvalue) 6e+03 1e+01 (Variables|/Game/DATA/Blueprints/Components/CombatComponent.CombatComponent_C|GetDraw%20Debug%20Type (Variables|Default|GetCombat%20Component)) false "WeaponEnd" (Variables|Default|GetCharacter)))
    (Game|SpawnActorfromClass "/Game/DATA/Blueprints/Actors/Magic/BP_Bullet.BP_Bullet_C" (Math|Transform|MakeTransform (Transformation|GetSocketLocation (Variables|/Game/DATA/Blueprints/Actors/BP_MasterItem.BP_MasterItem_C|GetItemSkeletalMesh _returnvalue) "BarrelSocket") (.rotation _returnvalue_2) "1.000000,1.000000,1.000000") "Undefined" "MultiplyWithRoot" _character (Variables|/Game/DATA/Blueprints/Actors/BP_BaseWeapon.BP_BaseWeapon_C|GetWeaponMultiplierDamage _returnvalue) 1e+01 2e+04 3e+04 _character (Variables|/Game/DATA/Blueprints/Actors/BP_BaseWeapon.BP_BaseWeapon_C|GetBasePoiseDamgeMultiplier _returnvalue) true (Variables|Default|GetSkill) false 0.0 _character)
    (CallFunction|Reset)
    (else
      (CallFunction|Reload))))

(event EventDone
  (params (Duration :type Float%20%28single-precision%29))
  ;[1 1 1] End GA
  (Utilities|FlowControl|RetriggerableDelay Duration)
  (Utilities|IsValid (Variables|Default|GetCharacter)
    (:Is%20Valid
      (CallFunction|FloatWeapon false "NewEnumerator2" "NewEnumerator2")
      (Default|RemoveGA (Variables|/Game/DATA/BP_PC.BP_PC_C|GetCombatComponent (Variables|Default|GetCharacter)) (Utilities|GetClass self))
      (Default|SetState (Variables|Default|GetCombat%20Component))
      (Actor|DestroyActor))))

(event EventTick
  (params (DeltaSeconds :type Float%20%28single-precision%29))
  ;[1 1 1] Spawn
  (bind _returnvalue (Default|RotatetoCamera (Variables|Default|GetTargetingComponent) 8.0))
  (if (<= _returnvalue 1.0)
    (Actor|Tick|SetActorTickEnabled false)))

(fn ConstructionScript
  (|CallParentFunction))

(fn Hold?
  (return (and (Utilities|Enum|Equal(Enum) (.State (Default|GetKeyStates (Variables|Default|GetCharacter) (Variables|Default|GetKeyIndex))) "NewEnumerator1") (Default|GetCurrentStateNotEqualAny (Variables|Default|GetCombat%20Component) "(GameplayTags=((TagName=\"Character.Action.Skill/Magic.Jump\"),(TagName=\"Character.State.Dodging\"),(TagName=\"Character.Action.Stuned\"),(TagName=\"Character.State.Attacking\"),(TagName=\"Character.State.Dead\"),(TagName=\"Character.State.Disabled\")))"))))

(fn FireAnimation
  (Animation|PlayAnimMontage (Variables|Default|GetCharacter) (Utilities|Array|Get(acopy) (Variables|/Game/DATA/Blueprints/Actors/BP_BaseWeapon.BP_BaseWeapon_C|GetLightAttackMontages (Variables|Default|GetGun))) 1.0 "None")
  (return))

(fn SetCost
  (bind _skill (Variables|Default|GetSkill))
  (bind _stats_component (Variables|Default|GetStats%20Component))
  (bind (_combat_types _mana_cost _stamina_cost) (Default|GetSkillStats _stats_component _skill))
  (Default|SetActionCost (Variables|Default|GetStats%20Component) (Variables|Default|GetSkill) (Math|Conversions|ToFloat(Integer) (Math|Integer|Clamp(Integer) _stamina_cost 1 _stamina_cost)) (Math|Conversions|ToFloat(Integer) (Math|Integer|Clamp(Integer) _mana_cost 0 _mana_cost))))

(fn PlayBowSwingandArrowSound
  (Components|Activation|Activate (Variables|/Game/DATA/Blueprints/Actors/BP_BaseWeapon.BP_BaseWeapon_C|GetImpactSound (select (Utilities|Enum|Equal(Enum) (Variables|/Game/DATA/Blueprints/Actors/BP_BaseWeapon.BP_BaseWeapon_C|GetTwoHandedCombatType (Default|GetMainWeapon (Variables|Default|GetCombat%20Component))) "NewEnumerator5") (Default|GetMainWeapon (Variables|Default|GetCombat%20Component)) (Default|GetOffHandedWeapon (Variables|Default|GetCombat%20Component)))) true)
  (Components|Activation|Activate (Variables|/Game/DATA/Blueprints/Actors/BP_BaseSpell.BP_BaseSpell_C|GetFlySound (Variables|Default|GetArrow)) true)
  (Components|Activation|Activate (Variables|/Game/DATA/Blueprints/Actors/BP_BaseSpell.BP_BaseSpell_C|GetTrail (Variables|Default|GetArrow)) true))

(fn SetRotation
  (bind _arrow (Variables|Default|GetArrow))
  (bind _character (Variables|Default|GetCharacter))
  (bind _returnvalue (Transformation|GetActorRotation _character))
  (bind _returnvalue_2 (Default|GetAimTrace (Variables|Default|GetCombat%20Component) (Variables|/Game/DATA/BP_PC.BP_PC_C|GetFollowCamera (Variables|Default|GetCharacter)) (Variables|/Game/DATA/Blueprints/Actors/BP_BaseSpell.BP_BaseSpell_C|GetVisualEffect _arrow) 6e+03 2e+01 (Variables|/Game/DATA/Blueprints/Components/CombatComponent.CombatComponent_C|GetDraw%20Debug%20Type (Variables|Default|GetCombat%20Component)) false "LHFS" _arrow))
  (Transformation|SetActorRotation (Variables|Default|GetCharacter) (Math|Rotator|MakeRotator (.Roll (Math|Rotator|BreakRotator _returnvalue)) 0.0 (.yaw (Math|Interpolation|RInterpTo _returnvalue (.rotation _returnvalue_2) (Utilities|Time|GetWorldDeltaSeconds) (Variables|Default|GetTargetRotationInterp%20Speed))))))

(fn IsThereAnyAmmo
  (bind _character (Variables|Default|GetCharacter))
  (bind _equipmentcomponet (Variables|/Game/DATA/BP_PC.BP_PC_C|GetEquipmentComponet _character))
  (bind (_array_element _item_info _equiped_item _returnvalue) (Default|IsTypeEquiped _equipmentcomponet "NewEnumerator29"))
  (return _returnvalue _equiped_item))

(fn RemoveArrow
  (bind _character (Variables|Default|GetCharacter))
  (bind _character_2 (Variables|Default|GetCharacter))
  (bind _inventory (Variables|/Game/DATA/BP_PC.BP_PC_C|GetInventory _character))
  (bind _inventory_2 (Variables|/Game/DATA/BP_PC.BP_PC_C|GetInventory _character_2))
  (bind _mainwidget (Variables|/Game/DATA/Blueprints/Actors/Inventory/BP_Inventory.BP_Inventory_C|GetMainWidget _inventory_2))
  (bind _arrowslots (Variables|/Game/DATA/Blueprints/Actors/Inventory/BP_Inventory.BP_Inventory_C|GetArrowSlots _inventory))
  (bind _cw_equipmentwidget (Variables|/Game/DATA/UI/Inventory/WBP_MainWidget.WBP_MainWidget_C|GetCW_EquipmentWidget _mainwidget))
  (bind _cw_arrows (Variables|/Game/DATA/UI/Inventory/CW_EquipmentWidget.CW_EquipmentWidget_C|GetCW_Arrows _cw_equipmentwidget))
  (if (Variables|/Game/DATA/Blueprints/Components/CombatComponent.CombatComponent_C|GetIsPlayer (Variables|Default|GetCombat%20Component))
    (Default|RemoveItematIndexAlt _inventory 0 1 false _arrowslots)
    (if (Default|IsSlotEmptyAlt _inventory 0 _arrowslots)
      (Utilities|IsValid _cw_arrows
        (:Is%20Valid
          (Default|UnequipItem _cw_arrows false)
          (return)))
      (else
        (return)))
    (else
      (return))))

(fn GetArrowType
  (bind _character (Variables|Default|GetCharacter))
  (bind _equipmentcomponet (Variables|/Game/DATA/BP_PC.BP_PC_C|GetEquipmentComponet _character))
  (bind (_array_element _item_info _equiped_item _returnvalue) (Default|IsTypeEquiped _equipmentcomponet "NewEnumerator29"))
  (return (.class _array_element) _returnvalue))

(fn ChangeVisualArrow
  (params (Item%20Class :type BP%20Master%20Item%20Class%20Reference))
  (bind _arrow (Variables|Default|GetArrow))
  (bind _output_get (Variables|/Game/DATA/Blueprints/Actors/Magic/BP_BaseArrowSpell.BP_BaseArrowSpell_C|SetItem%20Class _arrow Item%20Class))
  (Components|StaticMesh|SetStaticMesh (Variables|/Game/DATA/Blueprints/Actors/BP_BaseSpell.BP_BaseSpell_C|GetVisualEffect _arrow) (.CustomDropMesh (Utilities|GetClassDefaults _output_get))))

(fn GetArrowsWeight
  (bind _equiped_arrows (Variables|Default|GetEquiped%20Arrows))
  (bind _substatsbuff (Variables|/Game/DATA/Blueprints/Actors/BP_MasterItem.BP_MasterItem_C|GetSubStatsBuff _equiped_arrows))
  (bind (_value _returnvalue) (Utilities|Map|Find _substatsbuff "NewEnumerator32"))
  (return (select _returnvalue _value 1.0)))

(fn GetGun
  (bind _combat_component (Variables|Default|GetCombat%20Component))
  (bind _returnvalue (Default|GetMainWeapon _combat_component))
  (bind _equipedoffhand (Default|GetOffHandedWeapon _combat_component))
  (bind _twohandedcombattype (Variables|/Game/DATA/Blueprints/Actors/BP_BaseWeapon.BP_BaseWeapon_C|GetTwoHandedCombatType _returnvalue))
  (bind _returnvalue_2 (Utilities|Enum|Equal(Enum) _twohandedcombattype "NewEnumerator6"))
  (bind _returnvalue_3 (select _returnvalue_2 _returnvalue _equipedoffhand))
  (return (Variables|/Game/DATA/Blueprints/Actors/BP_MasterItem.BP_MasterItem_C|GetItemSkeletalMesh _returnvalue_3) _returnvalue_3))

(fn AimUpAnimation
  (Animation|PlayAnimMontage (Variables|Default|GetCharacter) (Utilities|Array|Get(acopy) (Variables|/Game/DATA/Blueprints/Actors/BP_BaseWeapon.BP_BaseWeapon_C|GetLightAttackMontages (Variables|Default|GetGun)) 1) 1.0 "None")
  (return))

(fn GunAnimation
  (bind _itemskeletalmesh (CallFunction|GetGun))
  (bind _gun (Variables|Default|GetGun))
  (bind _returnvalue (Math|Vector|GetForwardVector _itemskeletalmesh))
  (bind _returnvalue_2 (Math|Conversions|RotationFromXVector _returnvalue))
  (bind (_roll _pitch _yaw) (Math|Rotator|BreakRotator _returnvalue_2))
  (Animation|Montage|MontagePlay (Components|SkeletalMesh|GetAnimInstance (.ItemSkeletalMesh (CallFunction|GetGun))) "/Game/Pistol/Weap_Pistol_Fire_Montage.Weap_Pistol_Fire_Montage" 1.0 "MontageLength" 0.0 true)
  (Niagara|SpawnSystematLocation "/Game/Pistol/Particles/Weapons/N_Shell.N_Shell" (Transformation|GetSocketLocation (.ItemSkeletalMesh (CallFunction|GetGun)) "SlideSocket"))
  (Niagara|SpawnSystematLocation "/Game/Pistol/Particles/Weapons/N_MuzzleFlash.N_MuzzleFlash" (Transformation|GetSocketLocation _itemskeletalmesh "BarrelSocket") (Math|Rotator|MakeRotator _roll _pitch (+ _yaw 9e+01)))
  (Audio|Components|Audio|Play (Variables|/Game/DATA/Blueprints/Actors/Weapons/BP_BaseGun.BP_BaseGun_C|GetGunBang (Variables|Default|GetGun)) 0.0)
  (Math|Integer|DecrementInt (Variables|/Game/DATA/Blueprints/Actors/Weapons/BP_BaseGun.BP_BaseGun_C|GetAmmo _gun)
    (:%20%20
      (Default|UpdateTex _gun))))

(fn GetAmmo
  (Variables|Default|GetGun
    (:then
      _)
    (:else
      (bind _asbp_base_gun (Utilities|Casting|CastToBP_BaseGun (.ReturnValue (CallFunction|GetGun))))
      (Variables|Default|SetGun _asbp_base_gun)))
  (return (>= (Variables|/Game/DATA/Blueprints/Actors/Weapons/BP_BaseGun.BP_BaseGun_C|GetAmmo (Variables|Default|GetGun)) 1)))

(fn ReloadAnimation
  (Animation|PlayAnimMontage (Variables|Default|GetCharacter) (Utilities|Array|Get(acopy) (Variables|/Game/DATA/Blueprints/Actors/BP_BaseWeapon.BP_BaseWeapon_C|GetLightAttackMontages (Variables|Default|GetGun)) 2) 1.0 "None")
  (return))