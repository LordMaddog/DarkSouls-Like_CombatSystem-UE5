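; Player Power Slash ability actor that performs a skill attack and launches a BP_PowerSlice.
; GAStart checks two stats against a threshold, then plays the combat component's slash montage at a stat-driven rate and sets the action state, or runs an OOMCheck on failure.
; A montage notify spawns the slice ahead of a character socket with damage, area and poise settings.
; The actor destroys itself after a delay following montage blend-out.
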(event EventBeginPlay
  (|CallParentFunction) ; This node is disabled and will not be called.\nDrag off pins to build functionality.
)

(event Collision|EventActorBeginOverlap
  (params (OtherActor :type Actor%20Object%20Reference)))

(event EventTick
  (params (DeltaSeconds :type Float%20%28single-precision%29)))

(event EventGAStart
  (bind _character (Variables|Default|GetCharacter))
  (bind _stats_component (Variables|Default|GetStats%20Component))
  (bind _character_2 (Variables|Default|GetCharacter))
  (bind _returnvalue (Transformation|GetActorForwardVector _character_2))
  (if (and (Default|StatGreaterThen _stats_component "NewEnumerator2" 1e+01) (Default|StatGreaterThen _stats_component "NewEnumerator4" 1e+01))
    (Animation|Montage|PlayMontage (Variables|/Script/Engine.Character|GetMesh (Variables|Default|GetCharacter)) (Variables|/Game/DATA/Blueprints/Components/CombatComponent.CombatComponent_C|GetPowerSlashAnimation (Variables|Default|GetCombat%20Component)) (Default|GetSubStats (Variables|Default|GetStats%20Component) "NewEnumerator19")
      (:then
        (Default|SetState (Variables|Default|GetCombat%20Component) "(TagName=\"Character.State.GenralActionState\")")
        (Default|SetCurrentAction (Variables|Default|GetCombat%20Component) "(TagName=\"Character.Action.Skill/Magic\")"))
      (:OnBlendOut
        (Utilities|FlowControl|Delay 3.0)
        (Actor|DestroyActor))
      (:OnNotifyBegin
        (Game|SpawnActorfromClass "/Game/DATA/Blueprints/Actors/Magic/BP_PowerSlice.BP_PowerSlice_C" (Math|Transform|MakeTransform (+ (* _returnvalue 1e+02) (Transformation|GetSocketLocation (Variables|/Script/Engine.Character|GetMesh _character_2) "RHFS")) (Math|Conversions|RotationFromXVector _returnvalue) "1.000000,1.000000,1.000000") "AlwaysSpawn" "MultiplyWithRoot" _character 1.2 1.2e+02 2e+02 0.0 _character 2.0 false _character)
        (Default|SetCurrentAction (Variables|Default|GetCombat%20Component) "(TagName=\"Character.Action.Skill/Magic.PowerSlash\")")))
    (else
      (Default|OOMCheck (Variables|Default|GetStats%20Component) 1e+01))))

(fn ConstructionScript
  (|CallParentFunction))