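; Player rock throw magic ability, run as a short-lived actor.
; On start it checks stamina, mana and combat readiness, then rotates to target and plays a combo montage.
; ActivateComboSkill floats the weapon away, sets the cost and spawns BP_ThrownRock along an aim trace, scaled by skill stats.
; A retriggerable delay, also entered when checks fail, then returns the weapon, removes the ability and destroys the actor.
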(event Custom|Done
  ;[1 1 1] End
  (Utilities|FlowControl|RetriggerableDelay 3.0)
  (CallFunction|FloatWeapon false "NewEnumerator1" "NewEnumerator0")
  (Default|RemoveGA (Variables|/Game/DATA/BP_PC.BP_PC_C|GetCombatComponent (Variables|Default|GetCharacter)) (Utilities|GetClass self))
  (Actor|DestroyActor))

(event EventBeginPlay
  (|CallParentFunction) ; This node is disabled and will not be called.\nDrag off pins to build functionality.
)

(event Collision|EventActorBeginOverlap
  (params (OtherActor :type Actor%20Object%20Reference)))

(event EventTick
  (params (DeltaSeconds :type Float%20%28single-precision%29)))

(event EventGAStart
  (bind _stats_component (Variables|Default|GetStats%20Component))
  (bind _stats_component_2 (Variables|Default|GetStats%20Component))
  (bind (_mana_cost _stamina_cost) (Default|GetSkillStats _stats_component_2 "(TagName=\"Character.Action.Skill/Magic.RockThrow\")"))
  ;[1 1 1] Start
  (if (Math|Boolean|ANDBoolean (Default|StatGreaterThen _stats_component "NewEnumerator2" (Math|Conversions|ToFloat(Integer) _stamina_cost)) (Default|StatGreaterThen _stats_component "NewEnumerator4" (Math|Conversions|ToFloat(Integer) _mana_cost)) (Default|CanProformCombat (Variables|Default|GetCombat%20Component)))
    (Default|RotatetoTarget (Variables|Default|GetCharacter))
    (Default|PerformComboAction (Variables|Default|GetCombat%20Component) false (Variables|Default|GetAttackMontages))
    (Default|SetState (Variables|Default|GetCombat%20Component) "(TagName=\"Character.State.GenralActionState\")")
    (else
      (Default|OOMCheck (Variables|Default|GetStats%20Component) (Math|Conversions|ToFloat(Integer) (.Stamina%20Cost (Default|GetSkillStats (Variables|Default|GetStats%20Component) "(TagName=\"Character.Action.Skill/Magic.RockThrow\")"))))
      (CallFunction|Done))))

(event EventActivateComboSkill
  (params (Hand :type E_Handed%20Enum :default "NewEnumerator0"))
  (bind _character (Variables|Default|GetCharacter))
  (bind _character_2 (Variables|Default|GetCharacter))
  (bind _stats_component (Variables|Default|GetStats%20Component))
  (bind _stats_component_2 (Variables|Default|GetStats%20Component))
  (bind (_mana_cost _stamina_cost _skill_xp _level_up_cost _skill_level _available_points _power _effectiveness) (Default|GetSkillStats _stats_component "(TagName=\"Character.Action.Skill/Magic.RockThrow\")"))
  (bind (_mana_cost_2 _stamina_cost_2) (Default|GetSkillStats _stats_component_2 "(TagName=\"Character.Action.Skill/Magic.RockThrow\")"))
  ;[1 1 1] Spawn
  (CallFunction|FloatWeapon true "NewEnumerator1" "NewEnumerator0")
  (CallFunction|Done)
  (Default|SetActionCost (Variables|Default|GetStats%20Component) "(TagName=\"Character.Action.Skill/Magic.RockThrow\")" (Math|Conversions|ToFloat(Integer) _stamina_cost_2) (Math|Conversions|ToFloat(Integer) _mana_cost_2))
  (Default|SetCurrentAction (Variables|Default|GetCombat%20Component) "(TagName=\"Character.Action.Skill/Magic.RockThrow\")")
  (bind _returnvalue (Default|GetAimTrace (Variables|Default|GetCombat%20Component) (Variables|/Game/DATA/BP_PC.BP_PC_C|GetFollowCamera _character_2) (Variables|/Script/Engine.Character|GetMesh _character_2) 6e+03 2e+01 (Variables|/Game/DATA/Blueprints/Components/CombatComponent.CombatComponent_C|GetDraw%20Debug%20Type (Variables|Default|GetCombat%20Component)) true "LHFS" (Variables|Default|GetCharacter)))
  (Game|SpawnActorfromClass "/Game/DATA/Blueprints/Actors/Magic/BP_ThrownRock.BP_ThrownRock_C" _returnvalue "Undefined" "MultiplyWithRoot" _character _power (* _power 1e+01) 6e+03 (* _effectiveness 2e+03) _character _effectiveness true "(TagName=\"Character.Action.Skill/Magic.RockThrow\")" _character))

(fn ConstructionScript
  (|CallParentFunction))