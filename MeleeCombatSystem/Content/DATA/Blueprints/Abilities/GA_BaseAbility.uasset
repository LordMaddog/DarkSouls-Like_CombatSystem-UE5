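; Base actor for player combat abilities, with stub start, stop and combo-skill events for children.
; On BeginPlay it caches the owning BP_PC's components and binds to combat component melee and combo-skill events.
; Helpers float weapons with magic-dependent Niagara hand effects and equip a temporary hyper-armor item with a stat buff.
; Done waits on a retriggerable delay, then restores weapons, removes armor, unregisters the ability and destroys the actor.
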(event Custom|Done
  ;[1 1 1] Resets every thing
  (Utilities|FlowControl|RetriggerableDelay 5.0)
  (CallFunction|FloatWeapon false "NewEnumerator2" "NewEnumerator0")
  (CallFunction|UnEquipHyperArmor)
  (Default|RemoveGA (Variables|/Game/DATA/BP_PC.BP_PC_C|GetCombatComponent (Variables|Default|GetCharacter)) (Utilities|GetClass self))
  (Variables|/Game/DATA/Blueprints/Actors/BP_BaseWeapon.BP_BaseWeapon_C|SetMeleSkillused (Default|GetMainWeapon (Variables|/Game/DATA/BP_PC.BP_PC_C|GetCombatComponent (Variables|Default|GetCharacter))) "")
  (Actor|DestroyActor))

(event Custom|StopTick
  ;[1 1 1] enable tick
  (Actor|Tick|SetActorTickEnabled false))

(event Custom|MeleeAttackCalled
  ;[1 1 1] Base Call to use melee
  (CallFunction|FloatWeapon false "NewEnumerator2" "NewEnumerator0"))

(event Custom|ActivateComboSkill
  (params (Hand :type E_Handed%20Enum :default "NewEnumerator0"))
  ;[1 1 1] Base Call to use anim active weapon notify
)

(event Custom|StartTick
  ;[1 1 1] enable tick
  (Actor|Tick|SetActorTickEnabled true))

(event Custom|StartAbility)

(event Custom|StopAbility)

(event EventBeginPlay
  ;[1 1 1] Start
  (bind _asbp_pc (Utilities|Casting|CastToBP_PC (Components|GetOwner)))
  (Variables|Default|SetCharacter _asbp_pc)
  (Variables|Default|SetMesh (Variables|/Script/Engine.Character|GetMesh _asbp_pc))
  (Variables|Default|SetCharacter%20Movement (Variables|/Script/Engine.Character|GetCharacterMovement _asbp_pc))
  (Variables|Default|SetStats%20Component (Variables|/Game/DATA/BP_PC.BP_PC_C|GetStatsComponent _asbp_pc))
  (Variables|Default|SetMotionWarping (Variables|/Game/DATA/BP_PC.BP_PC_C|GetMotionWarping _asbp_pc))
  (Variables|Default|SetTargetingComponent (Variables|/Game/DATA/BP_PC.BP_PC_C|GetTargetingComponent _asbp_pc))
  (bind _output_get (Variables|Default|SetCombat%20Component (Variables|/Game/DATA/BP_PC.BP_PC_C|GetCombatComponent _asbp_pc)))
  (EventDispatchers|BindEventtoMeleeAttacked _output_get (EventDispatchers|CreateEvent :!event Custom|MeleeAttackCalled))
  (EventDispatchers|BindEventtoComboSkillActivate (Variables|Default|GetCombat%20Component) (EventDispatchers|CreateEvent :!event Custom|ActivateComboSkill)))

(fn ConstructionScript)

(fn FloatWeapon
  (params (FloatAway :type Boolean) (Hand :type E_Handed%20Enum :default "NewEnumerator0") (MagicType :type E_MagicType%20Enum :default "NewEnumerator0"))
  (bind _combat_component (Variables|Default|GetCombat%20Component))
  (bind _returnvalue (Default|GetCombatEnabled _combat_component))
  (bind _returnvalue_2 (Default|GetMainWeapon _combat_component))
  (bind _equipedoffhand (Default|GetOffHandedWeapon _combat_component))
  (if FloatAway
    _
    (else
      (CallFunction|FloatBack FloatAway)))
  (switch Utilities|FlowControl|Switch|SwitchonE_Handed Hand
    (:NewEnumerator0
      (if (Math|Boolean|ANDBoolean (Utilities|IsValid _returnvalue_2) _returnvalue (not (.right (Variables|Default|GetActiveHands)))) :!label _label
        (Default|WeaponFloat _returnvalue_2 FloatAway)
        (Variables|Default|SetActiveHands (Utilities|Struct|MakeS_LeftRight FloatAway false)))
      (if FloatAway
        (Utilities|IsValid (Variables|Default|GetRHandEffect)
          (:Is%20Not%20Valid
            (switch Utilities|FlowControl|Switch|SwitchonE_MagicType MagicType
              (:NewEnumerator0
                (bind _returnvalue_3 (Niagara|SpawnSystemAttached "/Game/DATA/Effects/N_Fire_Hands.N_Fire_Hands" (Variables|Default|GetMesh) "RHFS" "0, 0, 0" "0, 0, 0" "KeepRelativeOffset" false :!label _label_2))
                (Variables|Default|SetRHandEffect _returnvalue_3))
              (:NewEnumerator2
                (goto _label_2))
              (:NewEnumerator5
                (goto _label_2))
              (:NewEnumerator4
                (bind _returnvalue_4 (Niagara|SpawnSystemAttached "/Game/DATA/Effects/N_Ice_Hands.N_Ice_Hands" (Variables|Default|GetMesh) "RHFS" "0, 0, 0" "0, 0, 0" "KeepRelativeOffset" false :!label _label_3))
                (Variables|Default|SetRHandEffect _returnvalue_4))
              (:NewEnumerator3
                (goto _label_3))
              (:NewEnumerator1
                (goto _label_3)))))
        (else
          (Utilities|IsValid (Variables|Default|GetRHandEffect)
            (:Is%20Valid
              (Components|DestroyComponent (Variables|Default|GetRHandEffect)))))))
    (:NewEnumerator1
      (if (Math|Boolean|ANDBoolean _returnvalue (Utilities|IsValid _equipedoffhand) (not (.left (Variables|Default|GetActiveHands)))) :!label _label_4
        (Default|WeaponFloat _equipedoffhand FloatAway)
        (Variables|Default|SetActiveHands (Utilities|Struct|MakeS_LeftRight false FloatAway)))
      (if FloatAway
        (Utilities|IsValid (Variables|Default|GetLHandEffect)
          (:Is%20Not%20Valid
            (switch Utilities|FlowControl|Switch|SwitchonE_MagicType MagicType
              (:NewEnumerator0
                (bind _returnvalue_5 (Niagara|SpawnSystemAttached "/Game/DATA/Effects/N_Fire_Hands.N_Fire_Hands" (Variables|Default|GetMesh) "LHFS" "0, 0, 0" "0, 0, 0" "KeepRelativeOffset" false :!label _label_5))
                (Variables|Default|SetLHandEffect _returnvalue_5))
              (:NewEnumerator2
                (goto _label_5))
              (:NewEnumerator5
                (goto _label_5))
              (:NewEnumerator4
                (bind _returnvalue_6 (Niagara|SpawnSystemAttached "/Game/DATA/Effects/N_Ice_Hands.N_Ice_Hands" (Variables|Default|GetMesh) "LHFS" "0, 0, 0" "0, 0, 0" "KeepRelativeOffset" false :!label _label_6))
                (Variables|Default|SetLHandEffect _returnvalue_6))
              (:NewEnumerator3
                (goto _label_6))
              (:NewEnumerator1
                (goto _label_6)))))
        (else
          (Utilities|IsValid (Variables|Default|GetLHandEffect)
            (:Is%20Valid
              (Components|DestroyComponent (Variables|Default|GetLHandEffect)))))))
    (:NewEnumerator2
      (Utilities|FlowControl|Sequence
        (:then_0
          (goto _label))
        (:then_1
          (goto _label_4))))))

(fn FloatBack
  (params (FloatAway :type Boolean))
  (bind _activehands (Variables|Default|GetActiveHands))
  (bind _combat_component (Variables|Default|GetCombat%20Component))
  (Utilities|FlowControl|Sequence
    (:then_0
      (if (.right _activehands)
        (Default|WeaponFloat (Default|GetMainWeapon _combat_component) FloatAway)))
    (:then_1
      (if (.left _activehands)
        (Default|WeaponFloat (Default|GetOffHandedWeapon _combat_component) FloatAway)))))

(fn EquipHyperArmor
  (if (not (.ReturnValue (Utilities|Map|Find (Variables|/Game/DATA/Blueprints/Components/EquipmentComponet.EquipmentComponet_C|GetEquiped (Variables|/Game/DATA/BP_PC.BP_PC_C|GetEquipmentComponet (Variables|Default|GetCharacter))) "/Game/DATA/Blueprints/Actors/Armor/BP_HyperArmor.BP_HyperArmor_C")))
    (bind _newequip (Default|EquipItem (Variables|/Game/DATA/BP_PC.BP_PC_C|GetEquipmentComponet (Variables|Default|GetCharacter)) "/Game/DATA/Blueprints/Actors/Armor/BP_HyperArmor.BP_HyperArmor_C" "NewEnumerator7"))
    (bind _output_get (Variables|Default|SetHyperArmor _newequip))
    (Utilities|Map|Add (Variables|/Game/DATA/Blueprints/Actors/BP_BaseEquippable.BP_BaseEquippable_C|GetSubStatsBuff (Variables|Default|GetHyperArmor)) "NewEnumerator35" (Default|GetSubStats (Variables|Default|GetStats%20Component) "NewEnumerator11"))))

(fn UnEquipHyperArmor
  (bind _hyperarmor (Variables|Default|GetHyperArmor))
  (Utilities|IsValid _hyperarmor
    (:Is%20Valid
      (Default|UnequipItem (Variables|/Game/DATA/BP_PC.BP_PC_C|GetEquipmentComponet (Variables|Default|GetCharacter)) _hyperarmor "/Game/DATA/Blueprints/Actors/Armor/BP_HyperArmor.BP_HyperArmor_C" false))))

(fn GetDeathTeleportLocation
  (return "0, 0, 0"))