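; Ability actor that toggles a magic-type enchantment on the character's main weapon.
; EnchantWeapon requires two stats to pass a threshold, otherwise calling OOSBlink on the stats component.
; Activation plays a montage at a stat-driven rate, sets the action state, and applies the enchantment on notify begin.
; Deactivating, or activating an already enchanted weapon, removes it immediately; either toggle destroys the actor after a delay.
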(event EventBeginPlay
  (|CallParentFunction) ; This node is disabled and will not be called.\nDrag off pins to build functionality.
)

(event EventEnchantWeapon
  (params (Activate? :type Boolean) (MagicType :type E_MagicType%20Enum :default "NewEnumerator0"))
  (if (Default|StatGreaterThen (Variables|Default|GetStats%20Component) "NewEnumerator2" 1e+01)
    (if (Default|StatGreaterThen (Variables|Default|GetStats%20Component) "NewEnumerator4" 1e+01)
      (if Activate?
        (if (not (Variables|/Game/DATA/Blueprints/Actors/BP_BaseWeapon.BP_BaseWeapon_C|GetEnchantment%20active (Default|GetMainWeapon (Variables|Default|GetCombat%20Component))))
          (Animation|Montage|PlayMontage (Variables|/Script/Engine.Character|GetMesh (Variables|Default|GetCharacter)) (Variables|/Game/DATA/Blueprints/Components/CombatComponent.CombatComponent_C|GetEnchantWeaponAnim (Variables|Default|GetCombat%20Component)) (Default|GetSubStats (Variables|Default|GetStats%20Component) "NewEnumerator19")
            (:then
              (Default|SetState (Variables|Default|GetCombat%20Component) "(TagName=\"Character.State.GenralActionState\")")
              (Default|SetCurrentAction (Variables|Default|GetCombat%20Component) "(TagName=\"Character.Action.Skill/Magic.EnchantWeapon\")"))
            (:OnNotifyBegin
              (Default|Enchantment (Default|GetMainWeapon (Variables|Default|GetCombat%20Component)) true MagicType)
              (Utilities|FlowControl|Delay 5.0)
              (Actor|DestroyActor)))
          (else
            (Default|Enchantment (Default|GetMainWeapon (Variables|Default|GetCombat%20Component)) false MagicType :!label _label)
            (Utilities|FlowControl|Delay 5.0)
            (Actor|DestroyActor)))
        (else
          (goto _label)))
      (else
        (Default|OOSBlink (Variables|Default|GetStats%20Component) false)))
    (else
      (Default|OOSBlink (Variables|Default|GetStats%20Component) true))))

(fn ConstructionScript
  (|CallParentFunction))