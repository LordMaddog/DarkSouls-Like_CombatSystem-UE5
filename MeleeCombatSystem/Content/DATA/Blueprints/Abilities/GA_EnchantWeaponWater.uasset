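; Gameplay ability actor that toggles a water-element enchantment on the character's main weapon.
; On start it draws the weapon if needed, skips one weapon combat type, checks mana and stamina, then plays the enchant montage with magic hand effects.
; A montage notify applies skill power and effect to the weapon and updates its buff stats; an already enchanted weapon is disenchanted instead.
; A retriggerable delay then removes and destroys the ability.
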(event Custom|TimedReset
  ;[1 1 1] Start
  (Utilities|FlowControl|DoOnce false) ; enters at Reset
)

(event Custom|DeActivate
  ;[1 1 1] Deactivate
  (Default|Enchantment (Default|GetMainWeapon (Variables|Default|GetCombat%20Component)) false (Variables|Default|GetElement) (.Effectiveness (Default|GetSkillStats (Variables|Default|GetStats%20Component) (Variables|Default|GetSkill))))
  (Utilities|Map|Add (Variables|/Game/DATA/Blueprints/Actors/BP_MasterItem.BP_MasterItem_C|GetVisualStatsBuff (Default|GetMainWeapon (Variables|Default|GetCombat%20Component))) "NewEnumerator8" 0.0)
  (Default|EquipedBuffStats (Default|GetMainWeapon (Variables|Default|GetCombat%20Component)))
  (Audio|PlaySoundatLocation (Variables|Default|GetDeactivationSound) (Transformation|GetWorldLocation (Variables|/Game/DATA/Blueprints/Actors/BP_BaseWeapon.BP_BaseWeapon_C|GetEffectLocation (Default|GetMainWeapon (Variables|Default|GetCombat%20Component)))) "0, 0, 0" 1.0 1.0 0.0 0 0 0 0)
  (CallFunction|Done 3.0)
  (Utilities|FlowControl|Delay 0.2)
  (CallFunction|TimedReset))

(event Custom|Activate
  (bind _stats_component (Variables|Default|GetStats%20Component))
  (bind _combat_component (Variables|Default|GetCombat%20Component))
  (bind _skill (Variables|Default|GetSkill))
  (bind _returnvalue (Default|GetMainWeapon _combat_component))
  (bind (_mana_cost _stamina_cost _skill_xp _level_up_cost _skill_xpspent _skill_level _available_points _power _effectiveness) (Default|GetSkillStats _stats_component _skill))
  ;[1 1 1] Activate
  (Audio|PlaySoundatLocation (Variables|Default|GetActivationSound) (Transformation|GetWorldLocation (Variables|/Game/DATA/Blueprints/Actors/BP_BaseWeapon.BP_BaseWeapon_C|GetEffectLocation (Default|GetMainWeapon (Variables|Default|GetCombat%20Component)))) "0, 0, 0" 1.0 1.0 0.0 0 0 0 0)
  (Utilities|FlowControl|Delay 0.2)
  (Default|EnchantPowerSet _returnvalue _power (* _effectiveness 0.01))
  (Variables|/Game/DATA/Blueprints/Actors/BP_BaseWeapon.BP_BaseWeapon_C|SetMagicSkillused _returnvalue (Variables|Default|GetSkill))
  (Default|Enchantment (Default|GetMainWeapon (Variables|Default|GetCombat%20Component)) true (Variables|Default|GetElement) (.Effectiveness (Default|GetSkillStats (Variables|Default|GetStats%20Component) (Variables|Default|GetSkill))))
  (Utilities|Map|Add (Variables|/Game/DATA/Blueprints/Actors/BP_MasterItem.BP_MasterItem_C|GetVisualStatsBuff (Default|GetMainWeapon (Variables|Default|GetCombat%20Component))) "NewEnumerator8" (Math|Conversions|ToFloat(Integer) (.Mana%20Cost (Default|GetSkillStats (Variables|Default|GetStats%20Component) (Variables|Default|GetSkill)))))
  (Default|EquipedBuffStats (Default|GetMainWeapon (Variables|Default|GetCombat%20Component)))
  (CallFunction|Done 3.0))

(event EventBeginPlay
  (|CallParentFunction) ; This node is disabled and will not be called.\nDrag off pins to build functionality.
)

(event EventGAStart
  ;[1 1 1] Start
  (Utilities|FlowControl|DoOnce false
    (:Completed
      (if (not (Utilities|Enum|Equal(Enum) (Variables|/Game/DATA/Blueprints/Actors/BP_BaseWeapon.BP_BaseWeapon_C|GetOneHandedCombatType (Default|GetMainWeapon (Variables|Default|GetCombat%20Component))) "NewEnumerator5"))
        (Utilities|IsCombatReady?
          (:Exit
            (if (not (Variables|/Game/DATA/Blueprints/Actors/BP_BaseWeapon.BP_BaseWeapon_C|GetEnchantment%20active (Default|GetMainWeapon (Variables|Default|GetCombat%20Component))))
              (if (CallFunction|CheckManaStamina)
                (if (Default|CanProformCombat (Variables|Default|GetCombat%20Component))
                  (CallFunction|Done 3.0)
                  (Animation|Montage|PlayMontage (Variables|/Script/Engine.Character|GetMesh (Variables|Default|GetCharacter)) (Variables|/Game/DATA/Blueprints/Components/CombatComponent.CombatComponent_C|GetEnchantWeaponAnim (Variables|Default|GetCombat%20Component)) (Default|GetSubStats (Variables|Default|GetStats%20Component) "NewEnumerator19")
                    (:then
                      (Default|SetState (Variables|Default|GetCombat%20Component) "(TagName=\"Character.State.GenralActionState\")")
                      (Default|SetActionCost (Variables|Default|GetStats%20Component) (Variables|Default|GetSkill) 0.0 (Math|Conversions|ToFloat(Integer) (.Mana%20Cost (Default|GetSkillStats (Variables|Default|GetStats%20Component) (Variables|Default|GetSkill)))))
                      (Default|SetCurrentAction (Variables|Default|GetCombat%20Component) (Variables|Default|GetSkill))
                      (CallFunction|MagicHands "NewEnumerator0" (Variables|Default|GetElement) true)
                      (Utilities|FlowControl|Delay 0.2)
                      (CallFunction|TimedReset))
                    (:OnNotifyBegin
                      (CallFunction|Activate)))
                  (else
                    (Utilities|FlowControl|Delay 0.6 :!label _label)
                    (CallFunction|TimedReset)))
                (else
                  (Default|OOMCheck (Variables|Default|GetStats%20Component) (Math|Conversions|ToFloat(Integer) (.Mana%20Cost (Default|GetSkillStats (Variables|Default|GetStats%20Component) (Variables|Default|GetSkill)))))
                  (if (not (Variables|/Game/DATA/Blueprints/Actors/BP_BaseWeapon.BP_BaseWeapon_C|GetEnchantment%20active (Default|GetMainWeapon (Variables|Default|GetCombat%20Component))))
                    (CallFunction|Done 3.0)
                    (goto _label)
                    (else
                      (CallFunction|DeActivate)))))
              (else
                (CallFunction|DeActivate)))))))))

(event EventDone
  (params (Duration :type Float%20%28single-precision%29))
  ;[1 1 1] Done
  (Utilities|FlowControl|RetriggerableDelay Duration)
  (Default|RemoveGA (Variables|/Game/DATA/BP_PC.BP_PC_C|GetCombatComponent (Variables|Default|GetCharacter)) (Utilities|GetClass self))
  (CallFunction|MagicHands "NewEnumerator2" "NewEnumerator0" false)
  (Actor|DestroyActor))

(fn ConstructionScript
  (|CallParentFunction))

(fn CheckManaStamina
  (bind _stats_component (Variables|Default|GetStats%20Component))
  (bind _skill (Variables|Default|GetSkill))
  (bind _stats_component_2 (Variables|Default|GetStats%20Component))
  (bind (_mana_cost _stamina_cost) (Default|GetSkillStats _stats_component _skill))
  (return (and (Default|StatGreaterThen _stats_component_2 "NewEnumerator4" (Math|Conversions|ToFloat(Integer) _mana_cost)) (Default|StatGreaterThen _stats_component_2 "NewEnumerator2" (Math|Conversions|ToFloat(Integer) _stamina_cost)))))