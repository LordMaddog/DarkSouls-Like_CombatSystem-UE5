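; Player gameplay-ability actor for the tier-one Ice Spike spell, cast as a combat combo action.
; GAStart checks stamina, mana and combat readiness, then turns the character toward its target and plays a combo montage, or runs an out-of-mana check.
; ActivateComboSkill floats the weapon away, spawns BP_SpellIceT1 along a camera aim trace, scaled by skill stats, and deducts mana.
; Done uses a retriggerable delay before restoring weapons, unregistering and destroying itself.
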(event Custom|Done
  ;[1 1 1] Done self delete
  (Utilities|FlowControl|RetriggerableDelay 3.0)
  (CallFunction|FloatWeapon false "NewEnumerator2" "NewEnumerator0")
  (Default|RemoveGA (Variables|/Game/DATA/BP_PC.BP_PC_C|GetCombatComponent (Variables|Default|GetCharacter)) "GA_PlayerIceSpike_C")
  (Actor|DestroyActor))

(event EventBeginPlay
  (|CallParentFunction) ; This node is disabled and will not be called.\nDrag off pins to build functionality.
)

(event Collision|EventActorBeginOverlap
  (params (OtherActor :type Actor%20Object%20Reference)))

(event EventTick
  (params (DeltaSeconds :type Float%20%28single-precision%29)))

(event EventGAStart
  (bind _stats_component (Variables|Default|GetStats%20Component))
  (bind _stats_component_2 (Variables|Default|GetStats%20Component))
  (bind _stats_component_3 (Variables|Default|GetStats%20Component))
  (bind (_mana_cost _stamina_cost) (Default|GetSkillStats _stats_component_2 "(TagName=\"Character.Action.Skill/Magic.IceT1\")"))
  (bind (_mana_cost_2 _stamina_cost_2) (Default|GetSkillStats _stats_component_3 "(TagName=\"Character.Action.Skill/Magic.IceT1\")"))
  ;[1 1 1] Start
  (if (Math|Boolean|ANDBoolean (Default|StatGreaterThen _stats_component "NewEnumerator2" (Math|Conversions|ToFloat(Integer) _stamina_cost)) (Default|StatGreaterThen _stats_component "NewEnumerator4" (Math|Conversions|ToFloat(Integer) _mana_cost)) (Default|CanProformCombat (Variables|Default|GetCombat%20Component)))
    (if (>= (Default|GetSubStats (Variables|Default|GetStats%20Component) "NewEnumerator37") _mana_cost_2)
      (Default|RotatetoTarget (Variables|Default|GetCharacter))
      (Default|PerformComboAction (Variables|Default|GetCombat%20Component) false (Variables|Default|GetAttackMontages))
      (Default|SetState (Variables|Default|GetCombat%20Component) "(TagName=\"Character.State.GenralActionState\")")
      (else
        (Default|OOMCheck (Variables|Default|GetStats%20Component) 1e+04)
        (CallFunction|Done)))
    (else
      (Default|OOMCheck (Variables|Default|GetStats%20Component) (Math|Conversions|ToFloat(Integer) _stamina_cost_2))
      (CallFunction|Done))))

(event EventActivateComboSkill
  (params (Hand :type E_Handed%20Enum :default "NewEnumerator0"))
  (bind _character (Variables|Default|GetCharacter))
  (bind _character_2 (Variables|Default|GetCharacter))
  (bind _stats_component (Variables|Default|GetStats%20Component))
  (bind _stats_component_2 (Variables|Default|GetStats%20Component))
  (bind _stats_component_3 (Variables|Default|GetStats%20Component))
  (bind (_mana_cost _stamina_cost _skill_xp _level_up_cost _skill_level _available_points _power _effectiveness) (Default|GetSkillStats _stats_component "(TagName=\"Character.Action.Skill/Magic.IceT1\")"))
  (bind (_mana_cost_2 _stamina_cost_2) (Default|GetSkillStats _stats_component_2 "(TagName=\"Character.Action.Skill/Magic.IceT1\")"))
  (bind _mana_cost_3 (Default|GetSkillStats _stats_component_3 "(TagName=\"Character.Action.Skill/Magic.IceT1\")"))
  ;[1 1 1] Fire
  (switch Utilities|FlowControl|Switch|SwitchonE_Handed Hand
    (:NewEnumerator0
      (CallFunction|FloatWeapon true "NewEnumerator0" "NewEnumerator1"))
    (:NewEnumerator1
      (CallFunction|FloatWeapon true "NewEnumerator1" "NewEnumerator1"))
    (:NewEnumerator2
      (CallFunction|FloatWeapon true "NewEnumerator2" "NewEnumerator1")))
  (CallFunction|Done)
  (Default|SetActionCost (Variables|Default|GetStats%20Component) "(TagName=\"Character.Action.Skill/Magic.IceT1\")" (Math|Conversions|ToFloat(Integer) _stamina_cost_2) (Math|Conversions|ToFloat(Integer) _mana_cost_2))
  (Default|SetCurrentAction (Variables|Default|GetCombat%20Component) "(TagName=\"Character.Action.Skill/Magic.IceT1\")")
  (bind _returnvalue (Default|GetAimTrace (Variables|Default|GetCombat%20Component) (Variables|/Game/DATA/BP_PC.BP_PC_C|GetFollowCamera _character_2) (Variables|/Script/Engine.Character|GetMesh _character_2) 6e+03 2e+01 (Variables|/Game/DATA/Blueprints/Components/CombatComponent.CombatComponent_C|GetDraw%20Debug%20Type (Variables|Default|GetCombat%20Component)) true (select (Variables|Default|GetRightHanded) "LHFS" "RHFS") (Variables|Default|GetCharacter)))
  (Game|SpawnActorfromClass "/Game/DATA/Blueprints/Actors/Magic/BP_SpellIceT1.BP_SpellIceT1_C" _returnvalue "Undefined" "MultiplyWithRoot" _character _power (* (* _effectiveness 8e+01) _power) 6e+03 (* _effectiveness 3e+03) _character _effectiveness true "(TagName=\"Character.Action.Skill/Magic.IceT1\")" _character)
  (Audio|SpawnSoundatLocation "/Game/DATA/SoundFX/WaterMagic/SC_IceT1_cast.SC_IceT1_cast" (.Location (Math|Transform|BreakTransform _returnvalue)) "0, 0, 0" 1.0 1.0 0.0 0 0)
  (Default|ModifyCurrentSubStatValue (Variables|Default|GetStats%20Component) "NewEnumerator37" (* (Math|Integer|Clamp(Integer) _mana_cost_3 1 _mana_cost_3) -1.0)))

(fn ConstructionScript
  (|CallParentFunction))