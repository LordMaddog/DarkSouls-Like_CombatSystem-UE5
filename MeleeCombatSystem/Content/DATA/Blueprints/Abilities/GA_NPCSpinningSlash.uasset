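; NPC ability that performs a spinning slash melee skill with the main weapon, gated by two stat cost checks and combat availability.
; It rotates to the target, then a bounded retry loop draws the weapon until combat is enabled.
; It applies skill damage and poise multipliers, equips hyper armor, plays the combo montage and charges stamina and mana.
; The anim-notify-driven ActivateComboSkill event clears the weapon skill and removes hyper armor.
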(event EventBeginPlay
  (|CallParentFunction) ; This node is disabled and will not be called.\nDrag off pins to build functionality.
)

(event Collision|EventActorBeginOverlap
  (params (OtherActor :type Actor%20Object%20Reference)))

(event EventTick
  (params (DeltaSeconds :type Float%20%28single-precision%29)))

(event EventGAStart
  (bind _stats_component (Variables|Default|GetStats%20Component))
  (bind _skill (Variables|Default|GetSkill))
  (bind _skill_2 (Variables|Default|GetSkill))
  (bind _skill_3 (Variables|Default|GetSkill))
  (bind _stats_component_2 (Variables|Default|GetStats%20Component))
  (bind _stats_component_3 (Variables|Default|GetStats%20Component))
  (bind _stats_component_4 (Variables|Default|GetStats%20Component))
  (bind (_mana_cost _stamina_cost) (Default|GetSkillStats _stats_component_4 _skill_2))
  (bind (_mana_cost_2 _stamina_cost_2) (Default|GetSkillStats _stats_component_2 _skill_3))
  (bind (_mana_cost_3 _stamina_cost_3 _skill_xp _level_up_cost _skill_xpspent _skill_level _available_points _power _effectiveness) (Default|GetSkillStats _stats_component_3 _skill))
  ;[1 1 1] Slash
  (CallFunction|NPCGiveSkillifNoneExist "/Game/DATA/Blueprints/Actors/Useables/BP_SpinningSlashItem.BP_SpinningSlashItem_C" (Variables|Default|GetSkill))
  (if (Math|Boolean|ANDBoolean (Default|StatGreaterThen _stats_component "NewEnumerator2" (Math|Conversions|ToFloat(Integer) _stamina_cost_2)) (Default|StatGreaterThen _stats_component "NewEnumerator4" (Math|Conversions|ToFloat(Integer) _mana_cost_2)) (Default|CanProformCombat (Variables|Default|GetCombat%20Component)))
    (Default|RotatetoTarget (Variables|Default|GetCharacter))
    (Utilities|IsCombatReady?
      (:Exit
        (bind _output_get (Default|SetMeleeSkillUsed (Default|GetMainWeapon (Variables|/Game/DATA/BP_PC.BP_PC_C|GetCombatComponent (Variables|Default|GetCharacter))) (Variables|Default|GetSkill)))
        (Default|SetActionDamageMultiplyer (Default|GetMainWeapon (Variables|/Game/DATA/BP_PC.BP_PC_C|GetCombatComponent (Variables|Default|GetCharacter))) _output_get _power _effectiveness)
        (CallFunction|EquipHyperArmor)
        (Default|PerformComboAction (Variables|Default|GetCombat%20Component) false (Variables|Default|GetAttackMontages))
        (Default|SetState (Variables|Default|GetCombat%20Component) "(TagName=\"Character.State.GenralActionState\")")
        (Default|SetActionCost (Variables|Default|GetStats%20Component) (Variables|Default|GetSkill) (Math|Conversions|ToFloat(Integer) _stamina_cost) (Math|Conversions|ToFloat(Integer) _mana_cost))
        (Default|SetCurrentAction (Variables|Default|GetCombat%20Component) (Variables|Default|GetSkill))
        (CallFunction|Done 3.0)))
    (else
      (Default|OOMCheck (Variables|Default|GetStats%20Component) (Math|Conversions|ToFloat(Integer) (.Stamina%20Cost (Default|GetSkillStats (Variables|Default|GetStats%20Component) (Variables|Default|GetSkill)))))
      (CallFunction|Done 3.0))))

(event EventActivateComboSkill
  (params (Hand :type E_Handed%20Enum :default "NewEnumerator0"))
  ;[1 1 1] End through anim notify
  (CallFunction|Done 3.0)
  (Default|SetMeleeSkillUsed (Default|GetMainWeapon (Variables|/Game/DATA/BP_PC.BP_PC_C|GetCombatComponent (Variables|Default|GetCharacter))))
  (CallFunction|UnEquipHyperArmor))

(fn ConstructionScript
  (|CallParentFunction))