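; BP_AttackDamageType is a damage type Blueprint for attacks that exposes a DamageTypes value through its DamageType function.
; Its other functions, covering damage reception, desired rotation and combat attack, action and custom action requests, are stubs returning false, zero or a zero rotation.
; It runs no combat logic of its own, so DamageType is the only function that returns stored data.
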(fn CanReciveDamage
  (return false))

(fn DamageType
  (return (Variables|Default|GetDamageTypes)))

(fn GetDesiredRotation
  (return "0, 0, 0"))

(fn PreformCombatAction
  (params (ActionTag :type Gameplay%20Tag%20Structure) (SateTag :type Gameplay%20Tag%20Structure) (MontageIndex :type Integer) (bRandomItemIndex :type Boolean))
  (return 0.0))

(fn PreformCombatAttack
  (params (AttackType :type Gameplay%20Tag%20Structure) (SetState :type Gameplay%20Tag%20Structure) (AttackIndex :type Integer) (bRandomIndex :type Boolean))
  (return 0.0))

(fn PreformCustomAction
  (params (ActionTag :type Gameplay%20Tag%20Structure) (StateTag :type Gameplay%20Tag%20Structure) (InMontage :type Anim%20Montage%20Object%20Reference) (MontagePlayRate :type Float%20%28double-precision%29) (bAutoReset :type Boolean))
  (return false))