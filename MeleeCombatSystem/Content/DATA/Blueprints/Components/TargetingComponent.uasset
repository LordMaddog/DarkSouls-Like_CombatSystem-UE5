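; Lock-on targeting component for the BP_PC player character that finds a target and keeps the camera facing it.
; A sphere trace along the camera finds Targeting_BPI actors, which are notified and shift the camera boom while locked.
; Tick interpolates pitch-clamped control rotation toward the target unless player control is active, releasing invalid or out-of-range targets.
; It switches between strafing and movement-oriented rotation for sprints and dodges, and can turn the character toward the camera.
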(event Custom|DisableLockOn
  (CallFunction|SetTargeting false)
  (CallFunction|SetTargetActor)
  (CallFunction|SetRotationMode "NewEnumerator1")
  (Variables|/Script/Engine.SpringArmComponent|SetSocketOffset (Variables|/Game/DATA/BP_PC.BP_PC_C|GetCameraBoom (Variables|Default|GetOwnerCharacter)) "0.000000,50.000000,0.000000"))

(event Custom|EnableLockOn
  (bind (_returnvalue _foundtarget) (CallFunction|FindTarget))
  (if (and _returnvalue (CallFunction|CanTargetActor _foundtarget))
    (CallFunction|SetTargetActor _foundtarget)
    (CallFunction|SetTargeting true)
    (CallFunction|SetRotationMode "NewEnumerator0")
    (Variables|/Script/Engine.SpringArmComponent|SetSocketOffset (Variables|/Game/DATA/BP_PC.BP_PC_C|GetCameraBoom (Variables|Default|GetOwnerCharacter)) "0.000000,25.000000,0.000000")))

(event Custom|ToggleLockOn
  (if (CallFunction|Targeting?)
    (CallFunction|DisableLockon)
    (else
      (CallFunction|EnableLockon))))

(event Custom|TimedPlayerControl
  (bind _ownercharacter (Variables|Default|GetOwnerCharacter))
  (bind _action_value_x (Variables|/Game/DATA/BP_PC.BP_PC_C|GetAction%20Value%20X _ownercharacter))
  (if (or (> _action_value_x 1.0) (< _action_value_x -1.0))
    (CallFunction|SetPlayerControlStillActive true)
    (Utilities|FlowControl|RetriggerableDelay 0.1)
    (CallFunction|SetPlayerControlStillActive false)))

(event EventBeginPlay
  (bind _asbp_pc (Utilities|Casting|CastToBP_PC (Components|GetOwner)))
  (Variables|Default|SetOwnerCharacter _asbp_pc)
  (Variables|Default|SetOwnerControler (Pawn|GetController (Variables|Default|GetOwnerCharacter)))
  (Variables|Default|SetFollowCamera (Actor|GetComponentbyClass (Variables|Default|GetOwnerCharacter) "/Script/Engine.CameraComponent"))
  (Variables|Default|SetCombatComponent (Actor|GetComponentbyClass (Variables|Default|GetOwnerCharacter) "/Game/DATA/Blueprints/Components/CombatComponent.CombatComponent_C")))

(event EventTick
  (params (DeltaSeconds :type Float%20%28single-precision%29))
  (if (Variables|Default|GetAutoRotateCamera?)
    (CallFunction|RotatetoCameraTurn))
  (if (CallFunction|Targeting?)
    (CallFunction|UpdateTargetingControlRotation)))

(fn SetTargeting
  (params (bTargeting :type Boolean))
  (Variables|Default|SetbTargeting bTargeting)
  (bind _target_actor (Variables|Default|GetTarget%20Actor)
    (:then
      (Class|TargetingBPI|OnTargeted(Message) _target_actor bTargeting))
    (:else)))

(fn Targeting?
  (return (Variables|Default|GetbTargeting)))

(fn FindTarget
  (bind _ownercharacter (Variables|Default|GetOwnerCharacter))
  (bind _returnvalue (Transformation|GetActorLocation _ownercharacter))
  (bind (_outhit _returnvalue_2) (Collision|SphereTraceForObjects _returnvalue (+ (* (Math|Vector|GetForwardVector (Variables|Default|GetFollowCamera)) (Variables|Initialization|GetTargetingDistance)) _returnvalue) (Variables|Initialization|GetTargetRadius) (Variables|Initialization|GetTargetObject%20Types) false (Utilities|Array|MakeArray (Components|GetOwner)) (Variables|Initialization|GetDraw%20Debug%20Type)))
  (if (and _returnvalue_2 (Utilities|IsValid (.HitActor (Collision|BreakHitResult _outhit))))
    (if (Utilities|DoesObjectImplementInterface (.HitActor (Collision|BreakHitResult _outhit)) "/Game/DATA/Blueprints/Interface/Targeting_BPI.Targeting_BPI_C")
      (return true (.HitActor (Collision|BreakHitResult _outhit)))
      (else
        _)))
  (return false 0))

(fn SetTargetActor
  (params (NewTarget%20Actor :type Actor%20Object%20Reference))
  (Variables|Default|SetTarget%20Actor NewTarget%20Actor))

(fn GetTargetActor
  (return (Variables|Default|GetTarget%20Actor)))

(fn UpdateTargetingControlRotation
  (bind _returnvalue (Utilities|Time|GetWorldDeltaSeconds))
  (bind _target_actor (Variables|Default|GetTarget%20Actor))
  (bind _ownercontroler (Variables|Default|GetOwnerControler))
  (bind _ownercharacter (Variables|Default|GetOwnerCharacter))
  (bind _targetrotationinterp_speed (Variables|Default|GetTargetRotationInterp%20Speed))
  (bind _returnvalue_2 (Transformation|GetActorRightVector _ownercharacter))
  (bind _returnvalue_3 (Transformation|GetActorRotation _ownercontroler))
  (bind _returnvalue_4 (Transformation|GetActorLocation _ownercharacter))
  (bind _returnvalue_5 (Transformation|GetActorLocation _target_actor))
  (bind _returnvalue_6 (- _returnvalue_5 "0.000000,0.000000,50.000000"))
  (bind _returnvalue_7 (+ _returnvalue_2 _returnvalue_4))
  (bind _returnvalue_8 (Math|Rotator|FindLookatRotation _returnvalue_7 _returnvalue_6))
  (bind _returnvalue_9 (Math|Interpolation|RInterpTo _returnvalue_3 _returnvalue_8 _returnvalue _targetrotationinterp_speed))
  (if (and (Utilities|IsValid (Variables|Default|GetOwnerControler)) (not (CallFunction|GetPlayerControlStillActive)))
    (if (CallFunction|CanTargetActor (Variables|Default|GetTarget%20Actor))
      (CallFunction|KeepStrafing)
      (Pawn|SetControlRotation (Variables|Default|GetOwnerControler) (Math|Rotator|MakeRotator (.Roll (Math|Rotator|BreakRotator _returnvalue_3)) (Math|Float|Clamp(Float) (.pitch _returnvalue_9) -4e+01 4e+01) (.yaw _returnvalue_9)))
      (else
        (CallFunction|DisableLockon)))))

(fn SetRotationMode
  (params (RotationMode :type E_RotationMode%20Enum :default "NewEnumerator0"))
  (bind _output_get (Variables|Default|SetCurrentRotation%20Mode RotationMode))
  (switch Utilities|FlowControl|Switch|SwitchonE_RotationMode _output_get
    (:NewEnumerator0
      (Variables|/Script/Engine.Pawn|SetbUseControllerRotationYaw (Variables|Default|GetOwnerCharacter) true)
      (Variables|/Script/Engine.CharacterMovementComponent|SetbUseControllerDesiredRotation (Variables|/Script/Engine.Character|GetCharacterMovement (Variables|Default|GetOwnerCharacter)) true)
      (Variables|/Script/Engine.CharacterMovementComponent|SetbOrientRotationToMovement (Variables|/Script/Engine.Character|GetCharacterMovement (Variables|Default|GetOwnerCharacter)) false))
    (:NewEnumerator1
      (Variables|/Script/Engine.Pawn|SetbUseControllerRotationYaw (Variables|Default|GetOwnerCharacter) false)
      (Variables|/Script/Engine.CharacterMovementComponent|SetbUseControllerDesiredRotation (Variables|/Script/Engine.Character|GetCharacterMovement (Variables|Default|GetOwnerCharacter)) false)
      (Variables|/Script/Engine.CharacterMovementComponent|SetbOrientRotationToMovement (Variables|/Script/Engine.Character|GetCharacterMovement (Variables|Default|GetOwnerCharacter)) true))))

(fn GetRotationMode
  (return (Variables|Default|GetCurrentRotation%20Mode)))

(fn CanTargetActor
  (params (TargetActor :type Actor%20Object%20Reference))
  (Utilities|IsValid TargetActor
    (:Is%20Valid
      (bind _returnvalue (Class|TargetingBPI|CanbeTargeted(Message) TargetActor))
      (return (and _returnvalue (< (Transformation|GetDistanceTo (Components|GetOwner) TargetActor) (Variables|Initialization|GetTargetingDistance)))))
    (:Is%20Not%20Valid
      (return false))))

(fn UpdateRotationMode
  (Utilities|IsValid (Variables|Default|GetCombatComponent)
    (:Is%20Valid
      (CallFunction|SetRotationMode (select (Math|Boolean|ANDBoolean (not (Variables|/Game/DATA/Blueprints/Components/CombatComponent.CombatComponent_C|GetIs%20sprinting (Variables|Default|GetCombatComponent))) (Default|GetCombatEnabled (Variables|Default|GetCombatComponent)) (CallFunction|Targeting?)) "NewEnumerator1" (Variables|Default|GetCurrentRotation%20Mode))))
    (:Is%20Not%20Valid
      (Variables|Default|SetCombatComponent (Actor|GetComponentbyClass (Variables|Default|GetOwnerCharacter) "/Game/DATA/Blueprints/Components/CombatComponent.CombatComponent_C")))))

(fn GetPlayerControlStillActive
  (return (Variables|Default|GetPlayerControlStillActive)))

(fn SetPlayerControlStillActive
  (params (PlayerControlStillActive :type Boolean))
  (Variables|Default|SetPlayerControlStillActive PlayerControlStillActive))

(fn RotatetoTarget
  (bind _ownercharacter (Variables|Default|GetOwnerCharacter))
  (bind _ownercharacter_2 (Variables|Default|GetOwnerCharacter))
  (bind _returnvalue (Transformation|GetActorRotation _ownercharacter))
  (Transformation|SetActorRotation (Variables|Default|GetOwnerCharacter) (Math|Rotator|MakeRotator (.Roll (Math|Rotator|BreakRotator _returnvalue)) 0.0 (.yaw (Math|Interpolation|RInterpTo _returnvalue (Math|Rotator|FindLookatRotation (+ (* (Transformation|GetActorRightVector _ownercharacter_2) 3e+01) (Transformation|GetActorLocation _ownercharacter_2)) (- (Transformation|GetActorLocation (Variables|Default|GetTarget%20Actor)) "0.000000,0.000000,50.000000")) (Utilities|Time|GetWorldDeltaSeconds) (Variables|Default|GetTargetRotationInterp%20Speed))))))

(fn RotatetoCamera
  (params (InterpSpeed :type Float%20%28single-precision%29))
  (bind _followcamera (Variables|Default|GetFollowCamera))
  (bind _ownercharacter (Variables|Default|GetOwnerCharacter))
  (bind _ownercharacter_2 (Variables|Default|GetOwnerCharacter))
  (bind _returnvalue (Transformation|GetActorRotation _ownercharacter_2))
  (bind _returnvalue_2 (Math|Vector|GetForwardVector _followcamera))
  (bind _returnvalue_3 (Transformation|GetActorRotation _ownercharacter))
  (bind _returnvalue_4 (Math|Conversions|RotationFromXVector _returnvalue_2))
  (bind _yaw (Math|Rotator|BreakRotator _returnvalue_3))
  (bind _yaw_2 (Math|Rotator|BreakRotator _returnvalue_4))
  (bind _returnvalue_5 (- _yaw _yaw_2))
  (bind _returnvalue_6 (Math|Float|Absolute(Float) _returnvalue_5))
  (Transformation|SetActorRotation (Variables|Default|GetOwnerCharacter) (Math|Rotator|MakeRotator (.Roll (Math|Rotator|BreakRotator _returnvalue)) 0.0 (.yaw (Math|Interpolation|RInterpTo _returnvalue (Math|Conversions|RotationFromXVector (Math|Vector|GetForwardVector (Variables|Default|GetFollowCamera))) (Utilities|Time|GetWorldDeltaSeconds) InterpSpeed))))
  (Default|CallAimed (<= _returnvalue_6 1.0))
  (return _returnvalue_6))

(fn RotatetoCameraTurn
  (bind _ownercharacter (Variables|Default|GetOwnerCharacter))
  (bind _ownercharacter_2 (Variables|Default|GetOwnerCharacter))
  (bind _returnvalue (Transformation|GetActorRotation _ownercharacter))
  (bind _returnvalue_2 (Transformation|GetActorRotation _ownercharacter_2))
  (bind _returnvalue_3 (Pawn|GetControlRotation _ownercharacter_2 :!class /Script/Engine.Pawn))
  (bind _returnvalue_4 (Math|Rotator|Delta(Rotator) _returnvalue_3 _returnvalue_2))
  (if (> (.yaw _returnvalue_4) 1e+01)
    (Transformation|SetActorRotation (Variables|Default|GetOwnerCharacter) (Math|Rotator|MakeRotator (.Roll (Math|Rotator|BreakRotator _returnvalue)) 0.0 (.yaw (Math|Interpolation|RInterpTo _returnvalue (Math|Conversions|RotationFromXVector (Math|Vector|GetForwardVector (Variables|Default|GetFollowCamera))) (Utilities|Time|GetWorldDeltaSeconds) 4.0))) :!label _label)
    (elif (< (.yaw _returnvalue_4) -1e+01)
      (goto _label)
      (else
        (Variables|Default|SetAutoRotateCamera? false)
        (Class|AnimBPI|TurninPlace?(Message) (Components|SkeletalMesh|GetAnimInstance (Variables|/Script/Engine.Character|GetMesh (Variables|Default|GetOwnerCharacter))) false false)))))

(fn KeepStrafing
  (Utilities|IsValid (Variables|Default|GetCombatComponent)
    (:Is%20Valid
      (if (not (or (Variables|/Game/DATA/Blueprints/Components/CombatComponent.CombatComponent_C|GetIs%20sprinting (Variables|Default|GetCombatComponent)) (Default|GetCurrentStateEqual (Variables|Default|GetCombatComponent) "(TagName=\"Character.State.Dodging\")")))
        (CallFunction|SetRotationMode "NewEnumerator0")
        (else
          (CallFunction|SetRotationMode "NewEnumerator1"))))
    (:Is%20Not%20Valid
      (Variables|Default|SetCombatComponent (Actor|GetComponentbyClass (Variables|Default|GetOwnerCharacter) "/Game/DATA/Blueprints/Components/CombatComponent.CombatComponent_C")))))