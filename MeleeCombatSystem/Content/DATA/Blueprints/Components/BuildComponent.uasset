(event Custom|BuildDelay
  ;[1 1 1] BuildCycle
  (if (Variables|Default|GetIsBuildModeOn)
    (Utilities|FlowControl|Delay 0.01)
    (CallFunction|BuildCycle)
    (else
      (CallFunction|EndReset)
      (Utilities|IsValid (Variables|Default|GetBuildGhost)
        (:Is%20Valid
          (if (not (Variables|Default|GetReplaceMode))
            _
            (else
              (Default|SetMeshVisibility (Variables|Default|GetReplaceBuild) true)
              (Variables|Default|SetReplaceMode false)))
          (if (not (Variables|Default|GetMoveMode))
            (Default|DestroySelf (Variables|Default|GetBuildGhost) false)
            (else
              (Variables|Default|SetBuildGhost 0)
              (Variables|Default|SetMoveMode false))))))))

(event Custom|StopBuildMode
  ;[1 1 1] BuildCycle
  (CallFunction|EndReset)
  (Utilities|IsValid (Variables|Default|GetBuildGhost)
    (:Is%20Valid
      (if (not (Variables|Default|GetReplaceMode))
        _
        (else
          (Default|SetMeshVisibility (Variables|Default|GetReplaceBuild) true)
          (Variables|Default|SetReplaceMode false)))
      (if (not (Variables|Default|GetMoveMode))
        (Default|DestroySelf (Variables|Default|GetBuildGhost) false)
        (else
          (Variables|Default|SetBuildGhost 0)
          (Variables|Default|SetMoveMode false))))))

(event Custom|LaunchBuildMode
  ;[1 1 1] LaunchBuildMode
  (if (Variables|Default|GetIsBuildModeOn)
    (CallFunction|StopBuildMode)
    (else
      (Variables|Default|SetIsBuildModeOn true)
      (CallFunction|BuildCycle))))

(event Custom|LaunchMoveMode
  (params (BuildGhost :type BP%20Master%20Build%20Object%20Reference))
  ;[1 1 1] ActivateMoveMode
  (bind _output_get (Variables|Default|SetBuildGhost BuildGhost))
  (Default|SaveCurrentState _output_get)
  (Variables|Default|SetMoveMode true)
  (Variables|Default|SetIsBuildModeOn true)
  (CallFunction|BuildCycle))

(event Custom|ToggleFlip
  ;[1 1 1] ToggleFlip
  (if (Variables|Default|GetFlip)
    (Variables|Default|SetFlip false)
    (else
      (Variables|Default|SetFlip true))))

(event Custom|TogglePlaceAnywhere
  ;[1 1 1] Toggle Place Anywhere
  (if (Variables|Default|GetPlaceAnywhere)
    (Variables|Default|SetPlaceAnywhere false)
    (else
      (Variables|Default|SetPlaceAnywhere true))))

(event Custom|TogglePrecisePlaceing
  ;[1 1 1] Toggle PrecisePlacing
  (if (Variables|Default|GetPrecisePlacing)
    (Variables|Default|SetPrecisePlacing false)
    (else
      (Variables|Default|SetPrecisePlacing true))))

(event Custom|LaunchReplaceMode
  (params (BuildGhost :type BP%20Master%20Build%20Object%20Reference))
  ;[1 1 1] Launch Replacement Mode
  (bind _output_get (Variables|Default|SetBuildGhost BuildGhost))
  (Variables|Default|SetBuildSize (Variables|/Game/DATA/Blueprints/Actors/BuildItems/BP_MasterBuild.BP_MasterBuild_C|GetSize _output_get))
  (CallFunction|FindandSetBuildID)
  (Variables|Default|SetBuildTransform (Transformation|GetActorTransform (Variables|Default|GetBuildGhost)))
  (Variables|Default|SetReplaceMode true)
  (Variables|Default|SetPlaceAnywhere true)
  (Variables|Default|SetReplaceBuild (Variables|Default|GetBuildGhost))
  (Variables|Default|SetBuildGhost 0)
  (Variables|Default|SetIsBuildModeOn true)
  (CallFunction|BuildCycle))

(event Custom|ActiveDevMode
  (if (Variables|Default|GetDevMode)
    (Variables|Default|SetDevMode false)
    (else
      (Variables|Default|SetDevMode true)))
  (Development|PrintString (Utilities|String|Append "DevMode:" (Utilities|String|ToString(Boolean) (Variables|Default|GetDevMode)))))

(event EventBeginPlay
  ;[1 1 1] EventBeginPlay
  (bind _asbp_build_pawn (Utilities|Casting|CastToBP_BuildPawn (Components|GetOwner)))
  (Variables|Default|SetBuildPawn _asbp_build_pawn)
  (bind _outrownames (DataTable|GetDataTableRowNames "/Game/DATA/Blueprints/DataTables/DT_BuildItemList.DT_BuildItemList"))
  (for _array_element _outrownames
    (bind _returnvalue (Utilities|GetDataTableRow "/Game/DATA/Blueprints/DataTables/DT_BuildItemList.DT_BuildItemList" _array_element)
      (:then
        (Utilities|Array|Add (Variables|Default|GetBuildables) _returnvalue)))))

(fn SpawnBuildGost
  (bind _returnvalue (Game|SpawnActorfromClass (.buildactor (Utilities|Array|Get(acopy) (Variables|Default|GetBuildables) (Variables|Default|GetBuildID))) (Variables|Default|GetBuildTransform) "Undefined" "MultiplyWithRoot" 0 (LocalVariables|GetL_NotManualySpawned) (Variables|Default|GetBuildSize) false 0))
  (Variables|Default|SetBuildGhost _returnvalue)
  (Default|DisableAllColision (Variables|Default|GetBuildGhost))
  (Default|GiveBuildColor (Variables|Default|GetBuildGhost) (Variables|Default|GetCanBuild))
  (Transformation|SetActorTransform (Variables|Default|GetBuildGhost) (Variables|Default|GetBuildTransform) false true))

(fn BuildCycle
  (bind (_tstart _tend) (CallFunction|TraceStartEnd))
  (bind _buildghost (Variables|Default|GetBuildGhost))
  (bind _buildid (Variables|Default|GetBuildID))
  (bind _buildables (Variables|Default|GetBuildables))
  (bind _output (Utilities|Array|Get(acopy) _buildables _buildid))
  (if (not (Variables|Default|GetReplaceMode))
    (if (not (Variables|Default|GetPrecisePlacing))
      (bind (_outhit _returnvalue) (Collision|LineTraceByChannel _tstart _tend "TraceTypeQuery3" false (Utilities|Array|MakeArray (Variables|Default|GetBuildPawn) (Variables|Default|GetBuildGhost)) "None" :!label _label))
      (if _returnvalue
        (LocalVariables|SetL_HItActor (.HitActor (Collision|BreakHitResult _outhit)))
        (LocalVariables|SetL_HitComponent (.HitComponent (Collision|BreakHitResult _outhit)))
        (Math|Integer|IncrementInt (Variables|Default|GetTimedTest)
          (:%20%20
            (Variables|Default|SetBuildTransform (Math|Transform|MakeTransform (select (Math|Boolean|ORBoolean (Utilities|Enum|Equal(Enum) (.buildtype _output) "NewEnumerator5") (Utilities|Enum|Equal(Enum) (.buildtype _output) "NewEnumerator1") (Utilities|Enum|Equal(Enum) (.buildtype _output) "NewEnumerator6") (Utilities|Enum|Equal(Enum) (.buildtype _output) "NewEnumerator8") (Utilities|Enum|Equal(Enum) (.buildtype _output) "NewEnumerator7")) (+ (select _returnvalue (.ImpactPoint (Collision|BreakHitResult _outhit)) (.TraceEnd (Collision|BreakHitResult _outhit))) (Math|Vector|MakeVector 0.0 0.0 (Variables|Default|GetHeightOffset%20))) (select _returnvalue (.ImpactPoint (Collision|BreakHitResult _outhit)) (.TraceEnd (Collision|BreakHitResult _outhit)))) (.rotation (Variables|Default|GetBuildTransform)) (.scale (Variables|Default|GetBuildTransform))))
            (Utilities|IsValid _buildghost :!label _label_2
              (:Is%20Valid
                (bind (_hit_ _spawnloc) (CallFunction|DetectBuildBox (LocalVariables|GetL_HItActor) (LocalVariables|GetL_HitComponent)))
                (if _hit_
                  (Variables|Default|SetBuildTransform (Math|Transform|MakeTransform (.location _spawnloc) (.rotation _spawnloc) (CallFunction|GetSizeScale)))
                  (CallFunction|GetandChangeSize (LocalVariables|GetL_HItActor)))
                (Transformation|SetActorTransform (Variables|Default|GetBuildGhost) (Variables|Default|GetBuildTransform) false true)
                (if (not (Variables|Default|GetPlaceAnywhere))
                  (bind _returnvalue_2 (CallFunction|ChechforOverlap))
                  (bind _returnvalue_3 (CallFunction|CheckifFloating))
                  (Variables|Default|SetCanBuild (and (not _returnvalue_2) _returnvalue_3))
                  (else
                    (Variables|Default|SetCanBuild true)))
                (Default|GiveBuildColor (Variables|Default|GetBuildGhost) (Variables|Default|GetCanBuild))
                (CallFunction|BuildDelay))
              (:Is%20Not%20Valid
                (CallFunction|SpawnBuildGost :!label _label_3)
                (Transformation|SetActorTransform (Variables|Default|GetBuildGhost) (Variables|Default|GetBuildTransform) false true :!label _label_4)
                (CallFunction|BuildDelay)))))
        (else
          (Variables|Default|SetBuildTransform (Math|Transform|MakeTransform (select (Math|Boolean|ORBoolean (Utilities|Enum|Equal(Enum) (.buildtype _output) "NewEnumerator5") (Utilities|Enum|Equal(Enum) (.buildtype _output) "NewEnumerator1") (Utilities|Enum|Equal(Enum) (.buildtype _output) "NewEnumerator6") (Utilities|Enum|Equal(Enum) (.buildtype _output) "NewEnumerator8") (Utilities|Enum|Equal(Enum) (.buildtype _output) "NewEnumerator7")) (+ (select _returnvalue (.ImpactPoint (Collision|BreakHitResult _outhit)) (.TraceEnd (Collision|BreakHitResult _outhit))) (Math|Vector|MakeVector 0.0 0.0 (Variables|Default|GetHeightOffset%20))) (select _returnvalue (.ImpactPoint (Collision|BreakHitResult _outhit)) (.TraceEnd (Collision|BreakHitResult _outhit)))) (.rotation (Variables|Default|GetBuildTransform)) (.scale (Variables|Default|GetBuildTransform))))
          (Utilities|IsValid _buildghost
            (:Is%20Valid
              (bind _output_get (Variables|Default|SetCanBuild false))
              (Default|GiveBuildColor (Variables|Default|GetBuildGhost) _output_get)
              (goto _label_4))
            (:Is%20Not%20Valid
              (Variables|Default|SetCanBuild false)
              (goto _label_3)))))
      (elif (> (Variables|Default|GetTimedTest) 10)
        (goto _label_2)
        (else
          (goto _label))))
    (else
      (Utilities|IsValid (Variables|Default|GetBuildGhost)
        (:Is%20Valid
          (goto _label_2))
        (:Is%20Not%20Valid
          (CallFunction|SpawnBuildGost)
          (CallFunction|BuildDelay))))))

(fn ChangeActor
  (bind _buildghost (Variables|Default|GetBuildGhost))
  (Utilities|IsValid _buildghost
    (:Is%20Valid
      (if (not (== (.buildactor (Utilities|Array|Get(acopy) (Variables|Default|GetBuildables) (Variables|Default|GetBuildID))) (Utilities|GetClass _buildghost)))
        (Default|DestroySelf (Variables|Default|GetBuildGhost) false)))))

(fn PlaceBuild
  (if (Utilities|Enum|Equal(Enum) (.buildtype (Utilities|Array|Get(acopy) (Variables|Default|GetBuildables) (Variables|Default|GetBuildID))) "NewEnumerator1")
    (Default|AddFoundationExtension (Variables|Default|GetBuildGhost)))
  (if (not (Variables|Default|GetReplaceMode))
    _
    (else
      (Default|GiveBackandDestroySelf (Variables|Default|GetReplaceBuild))
      (Variables|Default|SetReplaceMode false)))
  (if (not (Variables|Default|GetMoveMode))
    (if (not (Variables|Default|GetDevMode))
      (Default|SetGrey (Variables|Default|GetBuildGhost))
      (else
        (Default|InGameManualyPlaceforBuilding (Variables|Default|GetBuildGhost))))
    (Variables|/Game/DATA/Blueprints/Actors/BuildItems/BP_MasterBuild.BP_MasterBuild_C|SetSize (Variables|Default|GetBuildGhost) (Variables|Default|GetBuildSize))
    (Default|SizeChange (Variables|Default|GetBuildGhost) false)
    (Variables|Default|SetBuildGhost 0)
    (else
      (Default|RestorCurrentState (Variables|Default|GetBuildGhost))
      (Variables|Default|SetBuildGhost 0)
      (Variables|Default|SetMoveMode false))))

(fn DetectBuildBox
  (params (Target :type Object%20Object%20Reference) (HitComponent :type Object%20Object%20Reference))
  (bind _return (Class|BuildBPI|BuildSnapLoc(Message) Target (.buildtype (Utilities|Array|Get(acopy) (Variables|Default|GetBuildables) (Variables|Default|GetBuildID))) "NewEnumerator0"))
  (bind _array_element (Utilities|Array|ForEachLoopwithBreak _return :!label _label)
    (:LoopBody
      (if (== (.Box (Utilities|Struct|BreakS_BuildSnapLoc _array_element)) HitComponent)
        (Utilities|IsValid (.SceneLoc (Utilities|Struct|BreakS_BuildSnapLoc _array_element))
          (:Is%20Valid
            (LocalVariables|SetL_SpawnLoc (Math|Transform|MakeTransform (.location (Transformation|GetWorldTransform (.SceneLoc (Utilities|Struct|BreakS_BuildSnapLoc _array_element)))) (select (Variables|Default|GetFlip) (Math|Conversions|RotationFromXVector (* (Math|Vector|GetForwardVector (.SceneLoc (Utilities|Struct|BreakS_BuildSnapLoc _array_element))) -1.0)) (.rotation (Transformation|GetWorldTransform (.SceneLoc (Utilities|Struct|BreakS_BuildSnapLoc _array_element))))) (.scale (Transformation|GetWorldTransform (.SceneLoc (Utilities|Struct|BreakS_BuildSnapLoc _array_element))))))
            (LocalVariables|SetL_Hit? true)
            (goto _label Break)))))
    (:Completed
      (return (Math|Boolean|ANDBoolean (LocalVariables|GetL_Hit?) (not (Variables|Default|GetPrecisePlacing)) (not (Variables|Default|GetReplaceMode))) (LocalVariables|GetL_SpawnLoc)))))

(fn RotateGhostBuild
  (params (Rotate :type Rotator))
  (if (Variables|Default|GetIsBuildModeOn)
    (Variables|Default|SetBuildTransform (Math|Transform|MakeTransform (.location (Variables|Default|GetBuildTransform)) (Math|Rotator|CombineRotators (.rotation (Variables|Default|GetBuildTransform)) Rotate) (.scale (Variables|Default|GetBuildTransform))))))

(fn ChechforOverlap
  (bind _buildghost (Variables|Default|GetBuildGhost))
  (bind _buildables (Variables|Default|GetBuildables))
  (bind _buildid (Variables|Default|GetBuildID))
  (bind _output (Utilities|Array|Get(acopy) _buildables _buildid))
  (bind _collisioncheckmesh (Variables|/Game/DATA/Blueprints/Actors/BuildItems/BP_MasterBuild.BP_MasterBuild_C|GetCollisionCheckMesh _buildghost))
  (bind (_origin _boxextent) (Collision|GetComponentBounds _collisioncheckmesh))
  (bind (_outhit _returnvalue) (Collision|BoxTraceByChannel _origin _origin (select (or (Utilities|Enum|Equal(Enum) (.buildtype _output) "NewEnumerator6") (Utilities|Enum|Equal(Enum) (.buildtype _output) "NewEnumerator8")) (* _boxextent 0.5) (* _boxextent 0.8)) "0, 0, 0" "TraceTypeQuery4" false (Utilities|Array|MakeArray _buildghost) "None" true "(R=1.000000,G=0.000000,B=0.000000,A=1.000000)" "(R=0.000000,G=1.000000,B=0.000000,A=1.000000)" 0.2))
  (if _returnvalue
    (bind _builditem (Class|BuildBPI|GetBuildItem(Message) (.HitActor (Collision|BreakHitResult _outhit))))
    (Utilities|IsValid _builditem
      (:Is%20Valid
        (if (Class|PrimitiveComponent|IsOverlappingComponent (Variables|/Game/DATA/Blueprints/Actors/BuildItems/BP_MasterBuild.BP_MasterBuild_C|GetCollisionCheckMesh _builditem) (Variables|/Game/DATA/Blueprints/Actors/BuildItems/BP_MasterBuild.BP_MasterBuild_C|GetCollisionCheckMesh (Variables|Default|GetBuildGhost)))
          (return true)
          (else
            (return false))))
      (:Is%20Not%20Valid
        (return true)))
    (else
      (return false))))

(fn CheckifFloating
  (bind _buildtransform (Variables|Default|GetBuildTransform))
  (bind _returnvalue (Collision|LineTraceByChannel (select (Utilities|Enum|Equal(Enum) (.buildtype (Utilities|Array|Get(acopy) (Variables|Default|GetBuildables) (Variables|Default|GetBuildID))) "NewEnumerator1") (+ (.location _buildtransform) "0.000000,0.000000,70.000000") (.location _buildtransform)) (+ (.location _buildtransform) "0.000000,0.000000,-500.000000") "TraceTypeQuery4" false (Utilities|Array|MakeArray (Variables|Default|GetBuildGhost)) "None"))
  (if (Utilities|Enum|Equal(Enum) (.buildtype (Utilities|Array|Get(acopy) (Variables|Default|GetBuildables) (Variables|Default|GetBuildID))) "NewEnumerator7")
    (return true)
    (else
      (return _returnvalue))))

(fn RaiseLower
  (params (OffsetIn :type Float%20%28double-precision%29))
  (Variables|Default|SetHeightOffset%20 (+ (Variables|Default|GetHeightOffset%20) OffsetIn)))

(fn ChangeSize
  (params (Value :type Integer))
  (bind _buildghost (Variables|Default|GetBuildGhost))
  (if (not (Variables|Default|GetMoveMode))
    (if (!= (Math|Integer|Clamp(Integer) (+ (Variables|Default|GetCurrentSize) Value) 0 4) (Variables|Default|GetCurrentSize))
      (bind _output_get (Variables|Default|SetCurrentSize (Math|Integer|Clamp(Integer) (+ (Variables|Default|GetCurrentSize) Value) 0 4)))
      (bind _output_get_2 (Variables|Default|SetBuildSize (Utilities|Select :Index _output_get :Option%200 "NewEnumerator1" :Option%201 "NewEnumerator2" :Option%202 "NewEnumerator3" :Option%203 "NewEnumerator4" :Option%204 "NewEnumerator5")))
      (Variables|Default|SetBuildTransform (Math|Transform|MakeTransform (.location (Variables|Default|GetBuildTransform)) (.rotation (Variables|Default|GetBuildTransform)) (CallFunction|GetSizeScale)))
      (Utilities|IsValid _buildghost
        (:Is%20Valid
          (Variables|/Game/DATA/Blueprints/Actors/BuildItems/BP_MasterBuild.BP_MasterBuild_C|SetSize _buildghost _output_get_2)
          (Default|SizeChange _buildghost false))))))

(fn GetSizeScale
  (switch Utilities|FlowControl|Switch|SwitchonE_BuildSize (Variables|Default|GetBuildSize)
    (:NewEnumerator1
      (return "0.500000,0.500000,0.500000"))
    (:NewEnumerator2
      (return "1.000000,1.000000,1.000000"))
    (:NewEnumerator3
      (return "1.500000,1.500000,1.500000"))
    (:NewEnumerator4
      (return "2.000000,2.000000,2.000000"))
    (:NewEnumerator5
      (return "3.000000,3.000000,3.000000"))))

(fn GetandChangeSize
  (params (Target :type Object%20Object%20Reference))
  (bind _buildghost (Variables|Default|GetBuildGhost))
  (bind _builditem (Class|BuildBPI|GetBuildItem(Message) Target))
  (if (Utilities|Enum|NotEqual(Enum) (Variables|/Game/DATA/Blueprints/Actors/BuildItems/BP_MasterBuild.BP_MasterBuild_C|GetSize _builditem) (Variables|Default|GetBuildSize))
    (bind _output_get (Variables|Default|SetBuildSize (Variables|/Game/DATA/Blueprints/Actors/BuildItems/BP_MasterBuild.BP_MasterBuild_C|GetSize _builditem)))
    (Variables|Default|SetBuildTransform (Math|Transform|MakeTransform (.location (Variables|Default|GetBuildTransform)) (.rotation (Variables|Default|GetBuildTransform)) (CallFunction|GetSizeScale)))
    (Utilities|IsValid _buildghost
      (:Is%20Valid
        (Variables|/Game/DATA/Blueprints/Actors/BuildItems/BP_MasterBuild.BP_MasterBuild_C|SetSize _buildghost _output_get)
        (Default|SizeChange _buildghost false))
      (:Is%20Not%20Valid
        _))
    (switch Utilities|FlowControl|Switch|SwitchonE_BuildSize (Variables|Default|GetBuildSize)
      (:NewEnumerator1
        (Variables|Default|SetCurrentSize 0))
      (:NewEnumerator2
        (Variables|Default|SetCurrentSize 1))
      (:NewEnumerator3
        (Variables|Default|SetCurrentSize 2))
      (:NewEnumerator4
        (Variables|Default|SetCurrentSize 3))
      (:NewEnumerator5
        (Variables|Default|SetCurrentSize 4)))))

(fn PreciseTransform
  (params (X :type Float%20%28double-precision%29) (y :type Float%20%28double-precision%29) (z :type Float%20%28double-precision%29))
  (Variables|Default|SetBuildTransform (Math|Transform|MakeTransform (Math|Vector|MakeVector (+ (.x (.location (Variables|Default|GetBuildTransform))) X) (+ y (.y (.location (Variables|Default|GetBuildTransform)))) (+ z (.z (.location (Variables|Default|GetBuildTransform))))) (.rotation (Variables|Default|GetBuildTransform)) (.scale (Variables|Default|GetBuildTransform)))))

(fn EndReset
  (Variables|Default|SetIsBuildModeOn false)
  (Variables|Default|SetCanBuild false)
  (Variables|Default|SetHeightOffset%20 0.0)
  (Variables|Default|SetLeftRightOffset 0.0)
  (Variables|Default|SetForwardBackOffset 0.0)
  (Variables|Default|SetTimedTest 0))

(fn TraceStartEnd
  (bind _buildpawn (Variables|Default|GetBuildPawn))
  (bind _camera (Variables|/Game/DATA/BP_BuildPawn.BP_BuildPawn_C|GetCamera _buildpawn))
  (bind _returnvalue (Math|Vector|GetForwardVector _camera))
  (bind _returnvalue_2 (Transformation|GetWorldLocation _camera))
  (return (+ _returnvalue_2 (* _returnvalue 1e+01)) (+ _returnvalue_2 (* _returnvalue 2e+03))))

(fn FindandSetBuildID
  (for (_array_element _array_index) (Variables|Default|GetBuildables)
    (if (== (.buildactor _array_element) (Utilities|GetClass (Variables|Default|GetBuildGhost)))
      (Variables|Default|SetBuildID _array_index))))

(fn ChangeBuildID
  (params (Value :type Integer))
  (if (not (Variables|Default|GetMoveMode))
    (LocalVariables|SetTempBuildID (Math|Integer|Clamp(Integer) (+ (Variables|Default|GetBuildID) Value) 0 (- (Utilities|Array|Length (Variables|Default|GetBuildables)) 1)))
    (if (not (Variables|Default|GetReplaceMode))
      (Variables|Default|SetBuildID (Math|Integer|Clamp(Integer) (+ (Variables|Default|GetBuildID) Value) 0 (- (Utilities|Array|Length (Variables|Default|GetBuildables)) 1)) :!label _label)
      (CallFunction|ChangeActor)
      (return)
      (elif (Utilities|Enum|Equal(Enum) (.Build%20Type (CallFunction|FindReplacementBuildID)) (.buildtype (Utilities|Array|Get(acopy) (Variables|Default|GetBuildables) (LocalVariables|GetTempBuildID))))
        (goto _label)
        (elif (== Value 1)
          (for (_array_element _array_index) (Variables|Default|GetBuildables)
            (if (and (Utilities|Enum|Equal(Enum) (.buildtype _array_element) (.Build%20Type (CallFunction|FindReplacementBuildID))) (> _array_index (LocalVariables|GetTempBuildID)))
              (Variables|Default|SetBuildID _array_index)
              (CallFunction|ChangeActor)
              (return)))
          (else
            (bind (_arrayindex _arrayelement) (Utilities|Array|ReverseforEachLoop (Variables|Default|GetBuildables))
              (:LoopBody
                (if (and (Utilities|Enum|Equal(Enum) (.buildtype _arrayelement) (.Build%20Type (CallFunction|FindReplacementBuildID))) (< _arrayindex (LocalVariables|GetTempBuildID)))
                  (Variables|Default|SetBuildID _arrayindex)
                  (CallFunction|ChangeActor)
                  (return))))))))))

(fn FindReplacementBuildID
  (for (_array_element _array_index) (Variables|Default|GetBuildables)
    (if (== (.buildactor _array_element) (Utilities|GetClass (Variables|Default|GetReplaceBuild)))
      (return _array_index (.buildtype _array_element)))))