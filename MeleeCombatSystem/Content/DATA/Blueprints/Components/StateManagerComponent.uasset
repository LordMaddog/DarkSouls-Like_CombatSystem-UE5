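; StateManagerComponent is a component that tracks a single current enum state.
; SetState ignores repeats of the current state, otherwise it broadcasts OnStateEnd for the old state, stores the new one and broadcasts OnStateBegin.
; ResetState writes the default enum value directly, without firing either event.
; Helpers return the current state or check whether it matches any in a given list.
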(fn SetState
  (params (NewSate :type E_CharactorState%20Enum :default "NewEnumerator0"))
  (if (Utilities|Enum|NotEqual(Enum) NewSate (Variables|Default|GetCurrentSate))
    (Default|CallOnStateEnd (Variables|Default|GetCurrentSate))
    (bind _output_get (Variables|Default|SetCurrentSate NewSate))
    (Default|CallOnStateBegin _output_get)))

(fn GetCurrentState
  (return (Variables|Default|GetCurrentSate)))

(fn ResetState
  (Variables|Default|SetCurrentSate "NewEnumerator0"))

(fn IsCurrentStateEqualtoAny
  (params (StatesToCheck :type Array%20of%20E_CharactorState%20Enums :default "NewEnumerator0"))
  (return (Utilities|Array|ContainsItem StatesToCheck (Variables|Default|GetCurrentSate))))