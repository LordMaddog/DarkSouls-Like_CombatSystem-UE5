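; Equipment component for BP_PC that spawns, tracks and removes the player's equipped item actors.
; Equipped items live in a class-keyed map; equipping unequips any same-type item (one type exempt), and gameplay tags locate items or trigger their actions.
; Changes refresh the inventory widget, player icon and quest widgets, then a retriggerable delay updates combat and blocking states.
; Retry loops wait for the Inventory reference and for item skill buffs to load.
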(event Custom|Update%20Inventory
  (params (EquipType :type E_EquipType%20Enum :default "NewEnumerator7") (Equipment :type BP%20Master%20Item%20Object%20Reference))
  (Utilities|IsValid (Variables|Default|GetInventory)
    (:Is%20Valid
      (Default|UpdateEquipType (Variables|/Game/DATA/UI/Inventory/WBP_MainWidget.WBP_MainWidget_C|GetCW_EquipmentWidget (Variables|/Game/DATA/Blueprints/Actors/Inventory/BP_Inventory.BP_Inventory_C|GetMainWidget (Variables|Default|GetInventory))) EquipType Equipment))))

(event Custom|UpDateDelay
  (bind _inventory (Variables|Default|GetInventory))
  (Utilities|IsValid _inventory
    (:Is%20Valid
      (Default|PlayerIconUpdate (Variables|/Game/DATA/Blueprints/Actors/Inventory/BP_Inventory.BP_Inventory_C|GetPlayer _inventory))
      (Utilities|FlowControl|Delay 0.1)
      (CallFunction|UpdateQuest))
    (:Is%20Not%20Valid
      _))
  (Utilities|FlowControl|RetriggerableDelay 0.4)
  (CallFunction|UpdateEquipStates))

(event Custom|CheckIfAllBuffsApplied
  (Utilities|GRDelay 0.5
    (:Completed
      (bind _return (CallFunction|SkillBuffsAdded))
      (if _return
        (Variables|Default|SetAllBuffsApplied true)
        (else
          (CallFunction|CheckifAllBuffsApplied))))))

(event EventBeginPlay
  (CallFunction|SetReferences)
  (bind _inventory (Utilities|GetInventory 1e+01)
    (:then
      (Variables|Default|SetInventory _inventory))))

(fn SetReferences
  (bind _asbp_pc (Utilities|Casting|CastToBP_PC (Components|GetOwner)))
  (Variables|Initalize|SetCharacter _asbp_pc)
  (Variables|Default|SetMesh (Variables|/Script/Engine.Character|GetMesh _asbp_pc))
  (Variables|Default|SetCharacter%20Movement (Variables|/Script/Engine.Character|GetCharacterMovement _asbp_pc))
  (Variables|Default|SetStats%20Component (Variables|/Game/DATA/BP_PC.BP_PC_C|GetStatsComponent _asbp_pc))
  (Variables|Default|SetMotionWarping (Variables|/Game/DATA/BP_PC.BP_PC_C|GetMotionWarping _asbp_pc))
  (Variables|Default|SetTargetingComponent (Variables|/Game/DATA/BP_PC.BP_PC_C|GetTargetingComponent _asbp_pc))
  (Variables|Default|SetCombat%20Component (Variables|/Game/DATA/BP_PC.BP_PC_C|GetCombatComponent _asbp_pc)))

(fn InitializeEquipment
  (for _array_element (Variables|Initalize|GetStartingEqupment)
    (if (Utilities|IsValidClass _array_element)
      (CallFunction|EquipItem _array_element (.DesiredEquipType (Utilities|GetClassDefaults _array_element)) (.ItemInfo (Utilities|GetClassDefaults _array_element)))))
  (return))

(fn PreformActionfromItem
  (params (ItemTag :type Gameplay%20Tag%20Container%20Structure))
  (bind _keys (Utilities|Map|Keys (Variables|Initalize|GetEquiped)))
  (for _array_element _keys
    (Utilities|IsValid (.equipeditem (.Value (Utilities|Map|Find (Variables|Initalize|GetEquiped) _array_element)))
      (:Is%20Valid
        (bind _returnvalue (Default|HasMatchingGamplayTag (.equipeditem (.Value (Utilities|Map|Find (Variables|Initalize|GetEquiped) _array_element))) ItemTag))
        (if _returnvalue
          (Default|PreformItemAction (.equipeditem (.Value (Utilities|Map|Find (Variables|Initalize|GetEquiped) _array_element))))))))
  (return))

(fn GetEquipedItembyTag
  (params (ItemTag :type Gameplay%20Tag%20Container%20Structure))
  (bind _keys (Utilities|Map|Keys (Variables|Initalize|GetEquiped)))
  (for _array_element _keys
    (Utilities|IsValid (.equipeditem (.Value (Utilities|Map|Find (Variables|Initalize|GetEquiped) _array_element)))
      (:Is%20Valid
        (bind _returnvalue (Default|HasMatchingGamplayTag (.equipeditem (.Value (Utilities|Map|Find (Variables|Initalize|GetEquiped) _array_element))) ItemTag))
        (if _returnvalue
          (return (.equipeditem (.Value (Utilities|Map|Find (Variables|Initalize|GetEquiped) _array_element)))))))))

(fn DestroyArmor&Equipment
  (params (DestroyActorToo? :type Boolean))
  (bind _combat_component (Variables|Default|GetCombat%20Component))
  (bind _returnvalue (Default|GetMainWeapon _combat_component))
  (Utilities|IsValid _returnvalue
    (:Is%20Valid
      (Actor|DestroyActor _returnvalue))
    (:Is%20Not%20Valid
      _))
  (bind _keys (Utilities|Map|Keys (Variables|Initalize|GetEquiped)))
  (for _array_element _keys
    (Utilities|IsValid (.equipeditem (.Value (Utilities|Map|Find (Variables|Initalize|GetEquiped) _array_element)))
      (:Is%20Valid
        (Actor|DestroyActor (.equipeditem (.Value (Utilities|Map|Find (Variables|Initalize|GetEquiped) _array_element))))
        (Utilities|Map|Remove (Variables|Initalize|GetEquiped) _array_element))))
  (if DestroyActorToo?
    (Actor|DestroyActor (Variables|Initalize|GetCharacter))))

(fn EquipItem
  (params (InEquipment :type BP%20Master%20Item%20Class%20Reference) (DesiredEquipType :type E_EquipType%20Enum :default "NewEnumerator7") (ItemInfo :type S%20Item%20Info%20Structure))
  (bind _character (Variables|Initalize|GetCharacter))
  (if (Utilities|IsValidClass InEquipment)
    (bind _returnvalue (Game|SpawnActorfromClass InEquipment (Transformation|GetActorTransform (Variables|Initalize|GetCharacter)) "Undefined" "MultiplyWithRoot" _character ItemInfo "NewEnumerator1" 1 DesiredEquipType "NewEnumerator2" 0 0 0 "NewEnumerator1" true _character))
    (Default|OnEquipped _returnvalue)
    (CallFunction|IsSameTypeOfCurrentlyEquiped InEquipment _returnvalue)
    (Utilities|Map|Add (Variables|Initalize|GetEquiped) InEquipment (Utilities|Struct|MakeS_EquippedItemInfo (Variables|/Game/DATA/Blueprints/Actors/BP_MasterItem.BP_MasterItem_C|GetEquipType _returnvalue) ItemInfo _returnvalue))
    (CallFunction|UpdateInventory (Variables|/Game/DATA/Blueprints/Actors/BP_MasterItem.BP_MasterItem_C|GetEquipType _returnvalue) _returnvalue)
    (CallFunction|UpDateDelay)
    (Default|PlayerIconUpdate (Variables|Initalize|GetCharacter))
    (return true _returnvalue)
    (else
      (return false 0))))

(fn UnequipItem
  (params (EquipmentToUnequip :type BP%20Master%20Item%20Object%20Reference) (ItemToUnequip :type BP%20Master%20Item%20Class%20Reference) (GiveBack? :type Boolean) (ForceDrop :type Boolean) (ItemInfoIn :type S%20Item%20Info%20Structure))
  (Utilities|IsValid EquipmentToUnequip
    (:Is%20Valid
      (Default|OnUnequipped EquipmentToUnequip GiveBack? ForceDrop ItemInfoIn)
      (CallFunction|UpDateDelay)
      (if (Utilities|IsValidClass ItemToUnequip)
        (Utilities|Map|Remove (Variables|Initalize|GetEquiped) ItemToUnequip)))))

(fn IsSameTypeOfCurrentlyEquiped
  (params (ItemIn :type BP%20Master%20Item%20Class%20Reference%20%28by%20ref%29) (EquipmentIn :type BP%20Master%20Item%20Object%20Reference))
  (bind _equiped (Variables|Initalize|GetEquiped))
  (bind _value (Utilities|Map|Find _equiped ItemIn))
  (if (Utilities|Enum|NotEqual(Enum) (Variables|/Game/DATA/Blueprints/Actors/BP_MasterItem.BP_MasterItem_C|GetEquipType EquipmentIn) "NewEnumerator7")
    (if (not (Utilities|Map|Contains (Variables|Initalize|GetEquiped) ItemIn))
      (bind _keys (Utilities|Map|Keys (Variables|Initalize|GetEquiped)))
      (for _array_element _keys
        (if (Utilities|Enum|Equal(Enum) (.equiptype (.Value (Utilities|Map|Find (Variables|Initalize|GetEquiped) _array_element))) (Variables|/Game/DATA/Blueprints/Actors/BP_MasterItem.BP_MasterItem_C|GetEquipType EquipmentIn))
          (CallFunction|UnequipItem (.equipeditem (.Value (Utilities|Map|Find (Variables|Initalize|GetEquiped) _array_element))) _array_element true false (.iteminfo (.Value (Utilities|Map|Find (Variables|Initalize|GetEquiped) _array_element))))))
      (return)
      (else
        (CallFunction|UnequipItem (.equipeditem _value) ItemIn true false (.iteminfo _value))
        (Default|CallUpdateInvalidEquipmentSlots)
        (return)))
    (else
      (return))))

(fn UpdateEquipStates
  (bind _keys (Utilities|Map|Keys (Variables|Initalize|GetEquiped)))
  (for _array_element _keys
    (if (Utilities|Enum|Equal(Enum) (Variables|/Game/DATA/Blueprints/Actors/BP_MasterItem.BP_MasterItem_C|GetEquipType (.equipeditem (.Value (Utilities|Map|Find (Variables|Initalize|GetEquiped) _array_element)))) "NewEnumerator23")
      (LocalVariables|SetL_CanDoCombat true)
      (elif (Utilities|Enum|Equal(Enum) (Variables|/Game/DATA/Blueprints/Actors/BP_MasterItem.BP_MasterItem_C|GetEquipType (.equipeditem (.Value (Utilities|Map|Find (Variables|Initalize|GetEquiped) _array_element)))) "NewEnumerator24")
        (LocalVariables|SetL_LeftHandWeapon true)
        (LocalVariables|SetL_LHW (.equipeditem (.Value (Utilities|Map|Find (Variables|Initalize|GetEquiped) _array_element)))))))
  (if (LocalVariables|GetL_CanDoCombat)
    (if (LocalVariables|GetL_LeftHandWeapon)
      (bind _asbp_base_weapon (Utilities|Casting|CastToBP_BaseWeapon (LocalVariables|GetL_LHW)))
      (Variables|Default|SetCan%20Block? (Variables|/Game/DATA/Blueprints/Actors/BP_BaseWeapon.BP_BaseWeapon_C|GetCanBlock? _asbp_base_weapon))
      (else
        (Variables|Default|SetCan%20Block? true)
        (Default|SetOffHandWeapon (Variables|/Game/DATA/BP_PC.BP_PC_C|GetCombatComponent (Variables|Initalize|GetCharacter)))))
    (else
      (Default|SetCombatEnabled (Variables|/Game/DATA/BP_PC.BP_PC_C|GetCombatComponent (Variables|Initalize|GetCharacter)) false)
      (Variables|Default|SetCan%20Block? false))))

(fn SkillBuffsAdded
  (bind _keys (Utilities|Map|Keys (Variables|Initalize|GetEquiped)))
  (for _array_element _keys
    (Utilities|IsValid (.equipeditem (.Value (Utilities|Map|Find (Variables|Initalize|GetEquiped) _array_element)))
      (:Is%20Valid
        (if (not (Variables|/Game/DATA/Blueprints/Actors/BP_MasterItem.BP_MasterItem_C|GetSkillBuffsFullyLoaded (.equipeditem (.Value (Utilities|Map|Find (Variables|Initalize|GetEquiped) _array_element)))))
          (return false)))))
  (return true))

(fn IsClassEquiped
  (params (Class :type BP%20Master%20Item%20Class%20Reference))
  (return (.ReturnValue (Utilities|Map|Find (Variables|Initalize|GetEquiped) Class))))

(fn UnequipClass
  (params (Class :type BP%20Master%20Item%20Class%20Reference))
  (bind _equiped (Variables|Initalize|GetEquiped))
  (bind _value (Utilities|Map|Find _equiped Class))
  (CallFunction|UnequipItem (.equipeditem _value) Class false false (.iteminfo _value)))

(fn ReEquipStartingEquipment
  (bind _keys (Utilities|Map|Keys (Variables|Initalize|GetEquiped)))
  (for _array_element _keys
    (CallFunction|UnequipItem (.equipeditem (.Value (Utilities|Map|Find (Variables|Initalize|GetEquiped) _array_element))) _array_element false false (.iteminfo (.Value (Utilities|Map|Find (Variables|Initalize|GetEquiped) _array_element)))))
  (for _array_element_2 (Variables|Initalize|GetStartingEqupment)
    (CallFunction|EquipItem _array_element_2 (.EquipType (Utilities|GetClassDefaults _array_element_2)) (.ItemInfo (Utilities|GetClassDefaults _array_element_2))))
  (return))

(fn UpdateQuest
  (bind _foundwidgets (Widget|GetAllWidgetsOfClass "/Game/DATA/UI/Inventory/QuestSubMenues/CW_ItemEquiped.CW_ItemEquiped_C" false))
  (for _array_element _foundwidgets
    (Class|UIBPI|GenericUpdate(Message) _array_element)))