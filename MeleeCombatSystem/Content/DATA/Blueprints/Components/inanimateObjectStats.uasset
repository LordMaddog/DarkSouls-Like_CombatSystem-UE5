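; Damage-receiving component for inanimate objects, caching its owner as either a world decoration or a player-build (BP_MasterBuild) actor.
; TakeDamge stores hit info, shows floating numbers, and forwards negated damage only to MasterBuild owners.
; A short retriggerable delay merges rapid hits into one number.
; CanReciveDamage returns true until Destroyed is set, while combat action, rotation and damage type functions are fixed-value stubs.
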(event EventBeginPlay
  (bind _returnvalue (Components|GetOwner))
  (bind _asbp_base_world_deco (Utilities|Casting|CastToBP_BaseWorldDeco _returnvalue)
    (:then
      (Variables|Default|SetWorld%20Deco _asbp_base_world_deco))
    (:CastFailed
      (bind _asbp_master_build (Utilities|Casting|CastToBP_MasterBuild _returnvalue))
      (Variables|Default|SetMaster%20Build _asbp_master_build))))

(event EventTick
  (params (DeltaSeconds :type Float%20%28single-precision%29)))

(event Custom|MakeFloatingNumbers
  (params (L%20DamageTaken :type Float%20%28double-precision%29))
  (bind _returnvalue (* L%20DamageTaken -1.0))
  (bind _world_deco (Variables|Default|GetWorld%20Deco))
  (Variables|Default|SetAddedDamage (+ (Variables|Default|GetAddedDamage) (Math|Float|Truncate _returnvalue)))
  (Utilities|FlowControl|RetriggerableDelay 0.05)
  (CallFunction|MakeFloatingNumbers (+ (Transformation|GetWorldLocation (select (Utilities|IsValid _world_deco) (Variables|/Game/DATA/Blueprints/Actors/BP_BaseWorldDeco.BP_BaseWorldDeco_C|GetStatBarWidget _world_deco) (Variables|/Game/DATA/Blueprints/Actors/BuildItems/BP_MasterBuild.BP_MasterBuild_C|GetDamageDisplayLoc (Variables|Default|GetMaster%20Build)))) "0.000000,0.000000,15.000000") (Variables|Default|GetAddedDamage) 0.5 (select (>= _returnvalue 1.0) false true))
  (Variables|Default|SetAddedDamage 0))

(event Custom|TakeDamge
  (params (Damage :type Float%20%28single-precision%29) (DamageType :type Damage%20Type%20Object%20Reference) (HitLocation :type Vector) (HitNormal :type Vector) (HitComponent :type Primitive%20Component%20Object%20Reference) (BoneName :type Name) (ShotFromDirection :type Vector) (InstigatedBy :type Controller%20Object%20Reference) (DamageCauser :type Actor%20Object%20Reference) (HitInfo :type Hit%20Result%20Structure%20%28by%20ref%29))
  (bind _master_build (Variables|Default|GetMaster%20Build))
  (CallFunction|DamageinInfo Damage DamageType DamageCauser HitInfo InstigatedBy)
  (CallFunction|MakeFloatingNumbers (Variables|Default|GetDamage%20In))
  (Utilities|IsValid _master_build
    (:Is%20Valid
      (Default|Damaged _master_build (* (Variables|Default|GetDamage%20In) -1.0) (.HitComponent (Collision|BreakHitResult (Variables|Default|GetDamageHit%20Info)))))))

(fn DamageinInfo
  (params (Damage :type Float%20%28single-precision%29) (Type :type Damage%20Type%20Object%20Reference) (Causer :type Actor%20Object%20Reference) (HitInfo :type Hit%20Result%20Structure%20%28by%20ref%29) (InstigatedBy :type Controller%20Object%20Reference))
  (Variables|Default|SetDamage%20Type Type)
  (Variables|Default|SetDamageHit%20Info HitInfo)
  (Variables|Default|SetDamage%20Causer Causer)
  (Variables|Default|SetDamage%20In Damage)
  (Variables|Default|SetInstigated%20By InstigatedBy))

(fn CanReciveDamage
  (return (not (Variables|Default|GetbDestroyed?))))

(fn DamageType
  (return "NewEnumerator0"))

(fn GetDesiredRotation
  (return "0, 0, 0"))

(fn PreformCombatAction
  (params (ActionTag :type Gameplay%20Tag%20Structure) (SateTag :type Gameplay%20Tag%20Structure) (MontageIndex :type Integer) (bRandomItemIndex :type Boolean))
  (return 0.0))

(fn PreformCombatAttack
  (params (AttackType :type Gameplay%20Tag%20Structure) (SetState :type Gameplay%20Tag%20Structure) (AttackIndex :type Integer) (bRandomIndex :type Boolean))
  (return 0.0))

(fn PreformCustomAction
  (params (ActionTag :type Gameplay%20Tag%20Structure) (StateTag :type Gameplay%20Tag%20Structure) (InMontage :type Anim%20Montage%20Object%20Reference) (MontagePlayRate :type Float%20%28double-precision%29) (bAutoReset :type Boolean))
  (return false))