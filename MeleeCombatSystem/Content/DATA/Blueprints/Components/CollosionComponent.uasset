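; Collision component that detects hits along a mesh while enabled, reporting each actor once per activation.
; Each tick it runs a multi-sphere object trace between start and end sockets on the assigned mesh, excluding an editable ignore list.
; New hit actors without ignored gameplay tags, queried by interface message, are recorded and broadcast through OnHit.
; Enabling collision clears the recorded actors, so they can be hit again.
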(event Custom|EnableCollision
  ;[1 1 1] Enable/DisableCollissions
  (CallFunction|ClearHitActors)
  (Variables|Traced|SetCollisionEnabled true))

(event Custom|DisableCollision
  ;[1 1 1] Enable/DisableCollissions
  (Variables|Traced|SetCollisionEnabled false))

(event Custom|CollisionTrace
  (bind _collisionmeshcomponent (Variables|Default|GetCollisionMeshComponent))
  ;[1 1 1] Trace
  (bind _outhits (Collision|MultiSphereTraceForObjects (Transformation|GetSocketLocation _collisionmeshcomponent (Variables|Initialization|GetStarSocket%20Name)) (Transformation|GetSocketLocation _collisionmeshcomponent (Variables|Initialization|GetEndSocket%20Name)) (Variables|Initialization|GetTraceRadius) (Variables|Initialization|GetCollisionObject%20Types) false (Variables|Initialization|GetActors%20to%20Ignore) (Variables|Initialization|GetDraw%20Debug%20Type)))
  (for _array_element _outhits
    (bind _output_get (Variables|Traced|SetLastHit _array_element))
    (if (CallFunction|GetHitActor (.HitActor (Collision|BreakHitResult _output_get)))
      (bind _output_get_2 (Variables|Traced|SetHit%20Actor (.HitActor (Collision|BreakHitResult _output_get))))
      (Utilities|Array|Add (Variables|Traced|GetAlreadyHitActors) _output_get_2)
      (Default|CallOnHit (Variables|Traced|GetLastHit)))))

(event Custom|ClearHitActors
  ;[1 1 1] Clear Actors
  (Utilities|Array|Clear (Variables|Traced|GetAlreadyHitActors)))

(event Custom|SetCollisionMesh
  (params (MeshComponent :type Primitive%20Component%20Object%20Reference))
  ;[1 1 1] SetMesh
  (Variables|Default|SetCollisionMeshComponent MeshComponent))

(event EventTick
  (params (DeltaSeconds :type Float%20%28single-precision%29))
  ;[1 1 1] Component Event tick
  (if (Variables|Traced|GetCollisionEnabled)
    (CallFunction|CollisionTrace)))

(fn GetAlreadyHitActors
  (return (Variables|Traced|GetAlreadyHitActors)))

(fn GetCollisionEnabled
  (return (Variables|Traced|GetCollisionEnabled)))

(fn GetLastHit
  (return (Variables|Traced|GetLastHit)))

(fn GetCollisionMeshcomponent
  (return (Variables|Default|GetCollisionMeshComponent)))

(fn AddActortoIgnore
  (params (InActor :type Actor%20Object%20Reference%20%28by%20ref%29))
  (Utilities|Array|AddUnique (Variables|Initialization|GetActors%20to%20Ignore) InActor))

(fn RemoveActortoIgnore
  (params (ActorToRemove :type Actor%20Object%20Reference%20%28by%20ref%29))
  (Utilities|Array|RemoveItem (Variables|Initialization|GetActors%20to%20Ignore) ActorToRemove))

(fn GetActorstoIgnore
  (return (Variables|Initialization|GetActors%20to%20Ignore)))

(fn GetHitActor
  (params (In%20actor :type Actor%20Object%20Reference))
  (bind _gameplaytags (Class|GameplayTagBPI|GetOwnedGamplayTags(Message) In%20actor))
  (return (and (not (Utilities|Array|ContainsItem (Variables|Traced|GetAlreadyHitActors) In%20actor)) (not (GameplayTags|HasAnyTags _gameplaytags (Variables|Default|GetGamplayTagsToIgnore) true)))))