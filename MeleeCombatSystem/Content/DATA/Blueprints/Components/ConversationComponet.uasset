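; Actor component that runs NPC dialogue with the player through the conversation graph system, adding a participant component when missing.
; It forwards reply options to the dialogue widget, advances on selection, and tracks a clamped stage that other conversations can unlock by tag.
; Dialogue hooks drive voice, montages, quest journal updates and random-rarity item rewards.
; A timer-driven camera zoom reattaches and interpolates the player's camera boom, then restores it.
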(event Custom|Chat
  (params (Player :type Actor%20Object%20Reference))
  (bind _actordialoguetag (Variables|Default|GetActorDialogueTag))
  ;[0.15 0.15 0.15 0.5] Start Dialogue
  (CallFunction|GetPlayerandUI Player)
  (CallFunction|InstalComponentUpdateUI)
  (Utilities|FlowControl|Delay 0.01)
  (Class|ConversationLibrary|StartConversationfromGraph _actordialoguetag (Components|GetOwner) _actordialoguetag (Variables|Initi|GetPlayer) (GameplayTags|MakeLiteralGameplayTag "(TagName=\"Character.Player\")") (Variables|Default|GetGraph)))

(event Custom|MoveCamera
  ;[0.15 0.15 0.15 0.5] Camera Zoom In
  (Utilities|FlowControl|Sequence
    (:then_0
      (Transformation|SetRelativeLocation (Variables|/Game/DATA/BP_PC.BP_PC_C|GetCameraBoom (Variables|Initi|GetPlayer)) (Math|Interpolation|VInterpTo (Variables|/Script/Engine.SceneComponent|GetRelativeLocation (Variables|/Game/DATA/BP_PC.BP_PC_C|GetCameraBoom (Variables|Initi|GetPlayer))) (Variables|Initi|GetMoveLoc) (Utilities|Time|GetWorldDeltaSeconds) 0.01) false true)
      (if (and (Utilities|Operators|EqualEqual (Variables|Initi|GetMoveLoc) (Variables|/Script/Engine.SceneComponent|GetRelativeLocation (Variables|/Game/DATA/BP_PC.BP_PC_C|GetCameraBoom (Variables|Initi|GetPlayer))) 1.0) (Variables|Initi|GetOffsetDone))
        (Utilities|Time|ClearandInvalidateTimerbyHandle (Variables|Initi|GetMoveTimer))))
    (:then_1
      (if (Variables|Initi|GetZoomingCamera)
        (Variables|Initi|SetOffsetDone true)
        (else
          (Variables|/Script/Engine.SpringArmComponent|SetSocketOffset (Variables|/Game/DATA/BP_PC.BP_PC_C|GetCameraBoom (Variables|Initi|GetPlayer)) (Math|Interpolation|VInterpTo (Variables|/Script/Engine.SpringArmComponent|GetSocketOffset (Variables|/Game/DATA/BP_PC.BP_PC_C|GetCameraBoom (Variables|Initi|GetPlayer))) (Variables|/Game/DATA/BP_PC.BP_PC_C|GetCameraBoomSocketOffset (Variables|Initi|GetPlayer)) (Utilities|Time|GetWorldDeltaSeconds) 0.005))
          (if (Utilities|Operators|EqualEqual (Variables|/Script/Engine.SpringArmComponent|GetSocketOffset (Variables|/Game/DATA/BP_PC.BP_PC_C|GetCameraBoom (Variables|Initi|GetPlayer))) (Variables|/Game/DATA/BP_PC.BP_PC_C|GetCameraBoomSocketOffset (Variables|Initi|GetPlayer)) 0.1)
            (Variables|Initi|SetOffsetDone true)
            (CallFunction|EndZoomReset)))))))

(event Custom|CameraZoomEnd
  (bind _player (Variables|Initi|GetPlayer))
  ;[0.15 0.15 0.15 0.5] Camera Zoom In
  (Transformation|DetachFromComponent (Variables|/Game/DATA/BP_PC.BP_PC_C|GetCameraBoom (Variables|Initi|GetPlayer)) "KeepWorld" "KeepWorld" "KeepWorld" true)
  (Transformation|AttachComponentToComponent (Variables|/Game/DATA/BP_PC.BP_PC_C|GetCameraBoom _player) (Variables|/Script/Engine.Character|GetCapsuleComponent _player) "None" "KeepWorld" "KeepWorld" "KeepWorld" true)
  (if (Utilities|Time|IsValidTimerHandle (Variables|Initi|GetMoveTimer))
    (Utilities|Time|ClearandInvalidateTimerbyHandle (Variables|Initi|GetMoveTimer)))
  (Variables|Initi|SetMoveLoc (.Location (Math|Transform|BreakTransform (Variables|/Game/DATA/BP_PC.BP_PC_C|GetDefaultCameraLoc (Variables|Initi|GetPlayer)))))
  (Variables|Initi|SetZoomingCamera false)
  (bind _returnvalue (Utilities|Time|SetTimerbyFunctionName 0 "MoveCamera" 0.0001 true))
  (Variables|Initi|SetMoveTimer _returnvalue)
  (Variables|Initi|SetOffsetDone false))

(event Custom|EndZoomReset
  (bind _player (Variables|Initi|GetPlayer))
  ;[0.15 0.15 0.15 0.5] Camera Zoom In
  (Utilities|FlowControl|DoOnce false ; enters at Reset
    (:Completed
      (Transformation|DetachFromComponent (Variables|/Game/DATA/BP_PC.BP_PC_C|GetCameraBoom (Variables|Initi|GetPlayer)) "KeepWorld" "KeepWorld" "KeepWorld" true)
      (Transformation|AttachComponentToComponent (Variables|/Game/DATA/BP_PC.BP_PC_C|GetCameraBoom _player) (Variables|/Script/Engine.Character|GetCapsuleComponent _player) "None" "KeepWorld" "KeepWorld" "KeepWorld" true)
      (if (Utilities|Time|IsValidTimerHandle (Variables|Initi|GetMoveTimer))
        (Utilities|Time|ClearandInvalidateTimerbyHandle (Variables|Initi|GetMoveTimer)))
      (Variables|Initi|SetMoveLoc (.Location (Math|Transform|BreakTransform (Variables|/Game/DATA/BP_PC.BP_PC_C|GetDefaultCameraLoc (Variables|Initi|GetPlayer)))))
      (Variables|Initi|SetZoomingCamera false)
      (bind _returnvalue (Utilities|Time|SetTimerbyFunctionName 0 "MoveCamera" 0.0001 true))
      (Variables|Initi|SetMoveTimer _returnvalue)
      (Variables|Initi|SetOffsetDone false))))

(event EventUpdateDialogueUI
  (params (Portrait :type Texture%202D%20Object%20Reference) (Name :type Text) (ChatTex :type Text) (KeyInstruction :type Text) (InputActionOne :type Input%20Action%20Object%20Reference) (InputActionTwo :type Input%20Action%20Object%20Reference) (Fade :type Boolean) (DisplayDuration :type Float%20%28double-precision%29))
  (bind _dialogewindow (Variables|Initi|GetDialogeWindow))
  ;[0.15 0.15 0.15 0.5] Update UI
  (Default|Update _dialogewindow Portrait Name ChatTex KeyInstruction InputActionOne InputActionTwo Fade DisplayDuration)
  (Widget|SetVisibility _dialogewindow "Visible"))

(event EventCameraZoom
  (params (Duration :type Float%20%28double-precision%29))
  (bind _player (Variables|Initi|GetPlayer))
  (bind _cameraboom (Variables|/Game/DATA/BP_PC.BP_PC_C|GetCameraBoom _player))
  ;[0.15 0.15 0.15 0.5] Camera Zoom In
  (Variables|Initi|SetDelayDuration Duration)
  (Utilities|IsValid (Variables|Initi|GetCameraZoomLoc)
    (:Is%20Valid
      (Variables|/Script/Engine.SpringArmComponent|SetSocketOffset _cameraboom "0, 0, 0")
      (Transformation|DetachFromComponent _cameraboom "KeepWorld" "KeepWorld" "KeepWorld" true)
      (Transformation|AttachComponentToComponent (Variables|/Game/DATA/BP_PC.BP_PC_C|GetCameraBoom (Variables|Initi|GetPlayer)) (Variables|Initi|GetCameraZoomLoc) "None" "KeepWorld" "KeepWorld" "KeepWorld" true)
      (Variables|Initi|SetMoveLoc "0, 0, 0")
      (Variables|Initi|SetZoomingCamera true)
      (if (Utilities|Time|IsValidTimerHandle (Variables|Initi|GetMoveTimer))
        (Utilities|Time|ClearandInvalidateTimerbyHandle (Variables|Initi|GetMoveTimer)))
      (bind _returnvalue (Utilities|Time|SetTimerbyFunctionName 0 "MoveCamera" 0.0001 true))
      (Variables|Initi|SetMoveTimer _returnvalue)
      (Utilities|FlowControl|RetriggerableDelay Duration)
      (CallFunction|CameraZoomEnd))))

(event EventBeginPlay
  ;[0.15 0.15 0.15 0.5] Event begin Play
  (Utilities|IsValid (Variables|Initi|GetParticipantComponent)
    (:Is%20Not%20Valid
      (bind _returnvalue (Game|AddComponentbyClass (Components|GetOwner) "/Script/CommonConversationRuntime.ConversationParticipantComponent"))
      (Variables|Initi|SetParticipantComponent _returnvalue))))

(event EventGenericBoolQuest
  (params (QuestName :type Name :default "None") (BoolName :type Name :default "None") (Bool :type Boolean))
  ;[0.15 0.15 0.15 0.5] UpdateGenericBool
  (Class|UIBPI|UpdateGenericBoolQuest(Message) (Variables|/Game/DATA/UI/Inventory/WBP_MainWidget.WBP_MainWidget_C|GetCW_Journal (Variables|/Game/DATA/Blueprints/Actors/Inventory/BP_Inventory.BP_Inventory_C|GetMainWidget (Variables|/Game/DATA/BP_PC.BP_PC_C|GetInventory (Variables|Initi|GetPlayer)))) QuestName BoolName Bool))

(event EventGiveQuest
  (params (QuestName :type Name :default "None"))
  ;[0.15 0.15 0.15 0.5] Give new Quest
  (Class|UIBPI|AddQuest(Message) (Variables|/Game/DATA/UI/Inventory/WBP_MainWidget.WBP_MainWidget_C|GetCW_Journal (Variables|/Game/DATA/Blueprints/Actors/Inventory/BP_Inventory.BP_Inventory_C|GetMainWidget (Variables|/Game/DATA/BP_PC.BP_PC_C|GetInventory (Variables|Initi|GetPlayer)))) QuestName))

(event EventConversationWorldInteract
  (params (Index :type Integer))
  ;[0.15 0.15 0.15 0.5] Conversation WorldInteract
  (Class|ConversationBPI|ConversationWorldInteract(Message) (Components|GetOwner) Index))

(event EventGiveItemtoPlayer
  (params (Class :type BP%20Master%20Item%20Class%20Reference) (Min :type Integer) (Max :type Integer))
  ;[0.15 0.15 0.15 0.5] GiveItemToPlayer
  (Utilities|FlowControl|DoOnce false :!label _label
    (:Completed
      (CallFunction|GenerateItem Class (Utilities|Enum|ByteToEnumE_Rarity (Math|Conversions|ToByte(Integer) (Math|Random|RandomIntegerinRange Min Max))))
      (Utilities|FlowControl|Delay 0.2)
      (goto _label Reset))))

(event EventAdvanceOtherMaxConversation
  (params (OtherConversation :type Gameplay%20Tag%20Structure) (MaxStage :type Integer))
  (CallFunction|UpdateOthereMaxStage OtherConversation MaxStage))

(event EventRemoteSetNewMaxStage
  (params (MaxStage :type Integer))
  (CallFunction|UpdateMaxStage MaxStage))

(event EventModifyStage
  (params (Value :type Integer))
  ;[0.15 0.15 0.15 0.5] ModifyStages
  (Variables|Initi|SetConversationStage (Math|Integer|Clamp(Integer) (+ (Variables|Initi|GetConversationStage) Value) 0 (Variables|Default|GetMaxStage))))

(event EventSetStage
  (params (Current :type Integer) (Max :type Integer))
  ;[0.15 0.15 0.15 0.5] ModifyStages
  (Variables|Initi|SetConversationStage Current)
  (Variables|Default|SetMaxStage Max))

(event EventPlayAnimation
  (params (Montage :type Anim%20Montage%20Object%20Reference))
  (bind _mesh (Variables|Initi|GetMesh))
  ;[0.15 0.15 0.15 0.5] Play Animation
  (Utilities|IsValid _mesh
    (:Is%20Valid
      (Animation|Montage|PlayMontage _mesh Montage))))

(event EventCameraEndZoom
  (bind _player (Variables|Initi|GetPlayer))
  ;[0.15 0.15 0.15 0.5] Camera Zoom In
  (Transformation|DetachFromComponent (Variables|/Game/DATA/BP_PC.BP_PC_C|GetCameraBoom (Variables|Initi|GetPlayer)) "KeepWorld" "KeepWorld" "KeepWorld" true)
  (Transformation|AttachComponentToComponent (Variables|/Game/DATA/BP_PC.BP_PC_C|GetCameraBoom _player) (Variables|/Script/Engine.Character|GetCapsuleComponent _player) "None" "KeepWorld" "KeepWorld" "KeepWorld" true)
  (if (Utilities|Time|IsValidTimerHandle (Variables|Initi|GetMoveTimer))
    (Utilities|Time|ClearandInvalidateTimerbyHandle (Variables|Initi|GetMoveTimer)))
  (Variables|Initi|SetMoveLoc (.Location (Math|Transform|BreakTransform (Variables|/Game/DATA/BP_PC.BP_PC_C|GetDefaultCameraLoc (Variables|Initi|GetPlayer)))))
  (Variables|Initi|SetZoomingCamera false)
  (bind _returnvalue (Utilities|Time|SetTimerbyFunctionName 0 "MoveCamera" 0.0001 true))
  (Variables|Initi|SetMoveTimer _returnvalue)
  (Variables|Initi|SetOffsetDone false))

(event EventForwardContext
  (params (Context :type Conversation%20Context%20Structure) (PayLoad :type Client%20Conversation%20Message%20Payload%20Structure))
  ;[0.15 0.15 0.15 0.5] Update Reply UI
  (bind _output_get (Variables|Initi|SetCurrentPay%20Load PayLoad))
  (Utilities|FlowControl|Delay 0.2)
  (for (_array_element _array_index) (.Options (Utilities|Struct|BreakClientConversationMessagePayload _output_get))
    (if (or (not (Utilities|Enum|Equal(Enum) (.ChoiceText (Utilities|Struct|BreakClientConversationOptionEntry _array_element)) (Utilities|Text|MakeLiteralText "Continue"))) (>= (Utilities|Array|Length (.Options (Utilities|Struct|BreakClientConversationMessagePayload _output_get))) 2))
      (Class|UIBPI|AddReplyChoice(Message) (Variables|Initi|GetDialogeWindow) _array_index (.ChoiceText (Utilities|Struct|BreakClientConversationOptionEntry _array_element))))))

(event EventCompleteQuest
  (params (QuestID :type Name :default "None"))
  ;[0.15 0.15 0.15 0.5] Complete Quest
  (Class|UIBPI|SetQuestComplete(Message) (Variables|/Game/DATA/UI/Inventory/WBP_MainWidget.WBP_MainWidget_C|GetCW_Journal (Variables|/Game/DATA/Blueprints/Actors/Inventory/BP_Inventory.BP_Inventory_C|GetMainWidget (Variables|/Game/DATA/BP_PC.BP_PC_C|GetInventory (Variables|Initi|GetPlayer)))) QuestID))

(event EventAdvanceConversation
  (params (Index :type Integer))
  (bind _currentpay_load (Variables|Initi|GetCurrentPay%20Load))
  (bind _options (Utilities|Struct|BreakClientConversationMessagePayload _currentpay_load))
  (bind _output (Utilities|Array|Get(acopy) _options Index))
  (bind (_choicetext _choicetags _choicetype _choicereference _extradata) (Utilities|Struct|BreakClientConversationOptionEntry _output))
  ;[0.15 0.15 0.15 0.5] Inact selected reply
  (if (Utilities|Array|IsValidIndex _options Index)
    (Utilities|FlowControl|DoOnce false :!label _label
      (:Completed
        (Class|ConversationParticipantComponent|RequestServerAdvanceConversation (Variables|Initi|GetParticipantComponent) (Utilities|Struct|MakeAdvanceConversationRequest _choicereference _extradata))
        (Utilities|FlowControl|Delay 0.2)
        (goto _label Reset)))))

(event EventPlayVoicedDialogue
  (params (Sound :type Sound%20Base%20Object%20Reference))
  (bind _audiocomponent (Variables|Initi|GetAudioComponent))
  ;[0.15 0.15 0.15 0.5] Play Voice Sound
  (Utilities|IsValid _audiocomponent
    (:Is%20Valid
      (Audio|Components|Audio|SetSound _audiocomponent Sound)
      (Audio|Components|Audio|Play _audiocomponent 0.0))))

(fn GetPlayerandUI
  (params (InActor :type Object%20Object%20Reference))
  (bind _character (Class|CombatBPI|GetCharacterInfo(Message) InActor))
  (bind _output_get (Variables|Initi|SetPlayer _character))
  (Variables|Initi|SetDialogeWindow (Variables|/Game/DATA/UI/Inventory/WBP_MainWidget.WBP_MainWidget_C|GetCW_DialogeText (Variables|/Game/DATA/Blueprints/Actors/Inventory/BP_Inventory.BP_Inventory_C|GetMainWidget (Variables|/Game/DATA/BP_PC.BP_PC_C|GetInventory _output_get))))
  (return))

(fn InstalComponentUpdateUI
  (Utilities|IsValid (Variables|Initi|GetParticipantComponent)
    (:Is%20Valid
      _)
    (:Is%20Not%20Valid
      (bind _returnvalue (Game|AddComponentbyClass (Components|GetOwner) "/Script/CommonConversationRuntime.ConversationParticipantComponent"))
      (Variables|Initi|SetParticipantComponent _returnvalue)))
  (Class|UIBPI|ShowInteractKeys(Message) (Variables|Initi|GetDialogeWindow) (Variables|Initi|GetParticipantComponent) self (Variables|Initi|GetPlayer)))

(fn GenerateItem
  (params (InputPin :type BP%20Master%20Item%20Class%20Reference) (Rarity :type E_Rarity%20Enum :default "NewEnumerator9"))
  (bind _player (Variables|Initi|GetPlayer))
  (bind _inventory (Variables|/Game/DATA/BP_PC.BP_PC_C|GetInventory _player))
  (bind _returnvalue (Game|SpawnActorfromClass InputPin (Math|Transform|MakeTransform "0, 0, 0" "0, 0, 0" "1.000000,1.000000,1.000000") "Undefined" "MultiplyWithRoot" 0 (.ItemInfo (Utilities|GetClassDefaults InputPin)) "NewEnumerator0" 1 "NewEnumerator7" "NewEnumerator0" 0 0 0 Rarity true 0))
  (Variables|/Game/DATA/Blueprints/Actors/BP_MasterItem.BP_MasterItem_C|SetGenerateRarity _returnvalue false)
  (Default|GenerateRarity _returnvalue 0.0)
  (Default|AutoDeleteSelf _returnvalue)
  (Default|AddItemAlt _inventory (Variables|/Game/DATA/Blueprints/Actors/BP_MasterItem.BP_MasterItem_C|GetItemInfo _returnvalue) InputPin 1 true (Variables|/Game/DATA/Blueprints/Actors/Inventory/BP_Inventory.BP_Inventory_C|GetSlots _inventory)))

(fn UpdateOthereMaxStage
  (params (Othere :type Gameplay%20Tag%20Structure) (MaxStageIn :type Integer))
  (bind _outactors (Actor|GetAllActorsOfClass "/Game/DATA/Blueprints/Actors/World/BP_ConversationNPCBase.BP_ConversationNPCBase_C"))
  (for _array_element _outactors
    (for _array_element_2 (Actor|GetComponentsByClass _array_element "ConversationComponet_C")
      (if (== (Variables|ConversationComponet_C|GetActorDialogueTag _array_element_2) Othere)
        (Class|ConversationBPI|RemoteSetNewMaxStage(Message) _array_element_2 MaxStageIn)
        (return)))))

(fn UpdateMaxStage
  (params (MaxStageIn :type Integer))
  (if (== (Variables|Default|GetMaxStage) (Variables|Initi|GetConversationStage))
    (Math|Integer|IncrementInt (Variables|Initi|GetConversationStage)
      (:%20%20
        _)))
  (Variables|Default|SetMaxStage MaxStageIn))

(fn CheckQuestComplete
  (params (QuestName :type Name :default "None"))
  (bind _cancomplete_ (Class|UIBPI|CanQuestComplete(Message) (Variables|/Game/DATA/UI/Inventory/WBP_MainWidget.WBP_MainWidget_C|GetCW_Journal (Variables|/Game/DATA/Blueprints/Actors/Inventory/BP_Inventory.BP_Inventory_C|GetMainWidget (Variables|/Game/DATA/BP_PC.BP_PC_C|GetInventory (Variables|Initi|GetPlayer)))) QuestName))
  (return _cancomplete_))

(fn EquipedDone
  (params (Quest :type Name :default "None"))
  (return false))

(fn GenBoolDone
  (params (QuestName :type Name :default "None") (BoolName :type Name :default "None"))
  (bind _value (Class|UIBPI|IsGenBoolDone(Message) (Variables|/Game/DATA/UI/Inventory/WBP_MainWidget.WBP_MainWidget_C|GetCW_Journal (Variables|/Game/DATA/Blueprints/Actors/Inventory/BP_Inventory.BP_Inventory_C|GetMainWidget (Variables|/Game/DATA/BP_PC.BP_PC_C|GetInventory (Variables|Initi|GetPlayer)))) QuestName BoolName))
  (return _value))

(fn GetConvoStage
  (return (Variables|Initi|GetConversationStage)))

(fn GetMerchant
  (return 0))

(fn GetTag
  (return (Variables|Default|GetActorDialogueTag)))