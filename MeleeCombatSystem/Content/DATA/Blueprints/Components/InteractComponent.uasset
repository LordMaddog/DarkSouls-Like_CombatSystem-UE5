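; Interact component that registers its owning actor in the player's nearby-interactables list and manages its prompt text.
; Start sets the text widget's label and color, while ToCastOrNotToCast filters for the player and caches it to avoid repeated lookups.
; Adding reveals the prompt only when the list is empty.
; Removing hides it, then checks the first remaining entry's sphere overlap, revealing its prompt or dropping it as stale.
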(event EventBeginPlay)

(event EventTick
  (params (DeltaSeconds :type Float%20%28single-precision%29)))

(fn ToCastorNottoCast
  (params (InActor :type Actor%20Object%20Reference))
  (Utilities|IsValid (Variables|Default|GetPlayer)
    (:Is%20Valid
      (if (== (Variables|Default|GetPlayer) InActor)
        _
        (else
          (return false))))
    (:Is%20Not%20Valid
      (bind _character (Class|CombatBPI|GetCharacterInfo(Message) InActor))
      (Utilities|IsValid _character
        (:Is%20Valid
          (if (Variables|/Game/DATA/Blueprints/Components/CombatComponent.CombatComponent_C|GetIsPlayer (Variables|/Game/DATA/BP_PC.BP_PC_C|GetCombatComponent _character))
            (Variables|Default|SetPlayer _character)
            (else
              (return false))))
        (:Is%20Not%20Valid
          (return false)))))
  (return true))

(fn AddtoInteractList
  (bind _interacttext (Variables|Default|GetInteractText))
  (if (> (Utilities|Array|Length (Variables|/Game/DATA/BP_PC.BP_PC_C|GetNearByActorsToInteract (Variables|Default|GetPlayer))) 0)
    _
    (else
      (Utilities|IsValid _interacttext
        (:Is%20Valid
          (Rendering|SetVisibility _interacttext true false))
        (:Is%20Not%20Valid
          _))))
  (if (not (Utilities|Array|ContainsItem (Variables|/Game/DATA/BP_PC.BP_PC_C|GetNearByActorsToInteract (Variables|Default|GetPlayer)) (Utilities|Struct|MakeS_NearByActorsToInteract (Variables|Default|GetOwningActor) (Variables|Default|GetInteractText))))
    (Utilities|Array|Add (Variables|/Game/DATA/BP_PC.BP_PC_C|GetNearByActorsToInteract (Variables|Default|GetPlayer)) (Utilities|Struct|MakeS_NearByActorsToInteract (Variables|Default|GetOwningActor) (Variables|Default|GetInteractText)))))

(fn RemovefromInteractList
  (if (> (Utilities|Array|Length (Variables|/Game/DATA/BP_PC.BP_PC_C|GetNearByActorsToInteract (Variables|Default|GetPlayer))) 0)
    (Utilities|IsValid (Variables|Default|GetInteractText)
      (:Is%20Valid
        (Rendering|SetVisibility (Variables|Default|GetInteractText) false false))
      (:Is%20Not%20Valid
        _))
    (Utilities|Array|RemoveItem (Variables|/Game/DATA/BP_PC.BP_PC_C|GetNearByActorsToInteract (Variables|Default|GetPlayer)) (Utilities|Struct|MakeS_NearByActorsToInteract (Variables|Default|GetOwningActor) (Variables|Default|GetInteractText)))
    (CallFunction|IsTextStillValid)
    (else
      (Utilities|Array|RemoveItem (Variables|/Game/DATA/BP_PC.BP_PC_C|GetNearByActorsToInteract (Variables|Default|GetPlayer)) (Utilities|Struct|MakeS_NearByActorsToInteract (Variables|Default|GetOwningActor) (Variables|Default|GetInteractText)))
      (Utilities|IsValid (Variables|Default|GetInteractText)
        (:Is%20Valid
          (Rendering|SetVisibility (Variables|Default|GetInteractText) false false))))))

(fn IsTextStillValid
  (bind _player (Variables|Default|GetPlayer))
  (bind _nearbyactorstointeract (Variables|/Game/DATA/BP_PC.BP_PC_C|GetNearByActorsToInteract _player))
  (bind _output (Utilities|Array|Get(acopy) _nearbyactorstointeract))
  (Utilities|IsValid (.actor _output)
    (:Is%20Valid
      (bind _item (Class|InteractableBPI|GetItemInfo(Message) (.actor _output)))
      (Utilities|IsValid _item
        (:Is%20Valid
          (if (Utilities|Array|ContainsItem (Collision|GetOverlappingActors (Variables|/Game/DATA/Blueprints/Actors/BP_MasterItem.BP_MasterItem_C|GetSphere _item) "/Game/DATA/BP_PC_Player.BP_PC_Player_C" :!class /Script/Engine.PrimitiveComponent) (Variables|Default|GetPlayer))
            (Rendering|SetVisibility (.text _output) true false)
            (return)
            (else
              _)))
        (:Is%20Not%20Valid
          _))
      (Rendering|SetVisibility (.text _output) false false)
      (Utilities|Array|RemoveItem (Variables|/Game/DATA/BP_PC.BP_PC_C|GetNearByActorsToInteract (Variables|Default|GetPlayer)) (Utilities|Struct|MakeS_NearByActorsToInteract (.actor _output) (.text _output)))
      (return))
    (:Is%20Not%20Valid
      (Utilities|Array|RemoveItem (Variables|/Game/DATA/BP_PC.BP_PC_C|GetNearByActorsToInteract (Variables|Default|GetPlayer)) (Utilities|Struct|MakeS_NearByActorsToInteract (.actor _output) (.text _output)))
      (return))))

(fn StartInteractText
  (bind _ascw_interact_text (Utilities|Casting|CastToCW_InteractText (UserInterface|GetUserWidgetObject (Variables|Default|GetInteractText))))
  (Rendering|Components|TextRender|SetText (Variables|/Game/DATA/UI/Inventory/CW_InteractText.CW_InteractText_C|GetNameText _ascw_interact_text) (Variables|Default|GetText))
  (Appearance|SetColorandOpacity (Variables|/Game/DATA/UI/Inventory/CW_InteractText.CW_InteractText_C|GetNameText _ascw_interact_text) (Utilities|Struct|MakeSlateColor (Variables|Default|GetTextColor)) :!class /Script/UMG.TextBlock))

(fn Start
  (params (OwningActor :type Actor%20Object%20Reference) (InteractText :type Widget%20Component%20Object%20Reference) (StartingText :type Text) (TextColor :type Linear%20Color%20Structure :default "(R=1.000000,G=1.000000,B=1.000000,A=1.000000)"))
  (Variables|Default|SetOwningActor OwningActor)
  (Variables|Default|SetInteractText InteractText)
  (Variables|Default|SetText StartingText)
  (Variables|Default|SetTextColor TextColor)
  (CallFunction|StartInteractText))

(fn PInteract
  (params (InActor :type Actor%20Object%20Reference))
  (bind _character (Class|CombatBPI|GetCharacterInfo(Message) InActor))
  (Variables|Default|SetPlayer _character)
  (return (Utilities|IsValid _character)))