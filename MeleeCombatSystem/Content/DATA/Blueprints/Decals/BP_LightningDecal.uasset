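; Lightning strike impact actor that leaves a fading decal with a physics impulse and hit sound.
; On BeginPlay it fires the radial force, plays the sound at a volume scaled by actor X scale, then fades the decal and destroys itself.
; A self-calling Shrink event steps down the smoke Niagara spawn rate, though nothing here starts it.
; An alternative trace-placed scorch decal is left unconnected.
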(event Custom|Shrink
  (Niagara|SetNiagaraVariable(Float) (Variables|Default|GetSmoke) "SpawnRate" (Variables|Default|GetSpawnRate))
  (Utilities|FlowControl|Delay 0.5)
  (bind _result (Math|Float|DecrementFloat (Variables|Default|GetSpawnRate))
    (:%20%20
      (if (> _result 0.0)
        (CallFunction|Shrink)))))

(event EventBeginPlay
  (bind _returnvalue (Transformation|GetActorScale3D))
  (bind _returnvalue_2 (* (.x _returnvalue) 0.05))
  (Utilities|FlowControl|Delay 0.0)
  (Class|RadialForceComponent|FireImpulse (Variables|Default|GetRadialForce))
  (Audio|Components|Audio|SetVolumeMultiplier (Variables|Default|GetHitSound) (Math|Float|Clamp(Float) _returnvalue_2 _returnvalue_2 1.5) :!class /Script/Engine.AudioComponent)
  (Rendering|Components|Decal|SetFadeOut (Variables|Default|GetDecal) 0.1 4e+01 true)
  (Components|Activation|Activate (Variables|Default|GetHitSound) false)
  (Utilities|FlowControl|Delay 4e+01)
  (Actor|DestroyActor))

(fn ConstructionScript)