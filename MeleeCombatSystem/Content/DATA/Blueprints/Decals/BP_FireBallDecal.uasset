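; BP_FireBallDecal is a decal actor with smoke, apparently left behind by a fireball.
; On BeginPlay the decal starts a long fade-out that destroys the actor when finished.
; In parallel, a Niagara smoke effect has its spawn rate lowered in timed steps until it reaches zero, looping through the Shrink event and a short delay.
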(event Custom|Shrink
  (Niagara|SetNiagaraVariable(Float) (Variables|Default|GetSmoke) "SpawnRate" (Variables|Default|GetSpawnRate))
  (Utilities|FlowControl|Delay 0.5)
  (bind _result (Math|Float|DecrementFloat (Variables|Default|GetSpawnRate))
    (:%20%20
      (if (> _result 0.0)
        (CallFunction|Shrink)))))

(event EventBeginPlay
  (Utilities|FlowControl|Sequence
    (:then_0
      (Rendering|Components|Decal|SetFadeOut (Variables|Default|GetDecal) 0.1 4e+01 true))
    (:then_1
      (Niagara|SetNiagaraVariable(Float) (Variables|Default|GetSmoke) "SpawnRate" (Variables|Default|GetSpawnRate))
      (Utilities|FlowControl|Delay 0.5)
      (bind _result (Math|Float|DecrementFloat (Variables|Default|GetSpawnRate))
        (:%20%20
          (if (> _result 0.0)
            (CallFunction|Shrink)))))))

(event Collision|EventActorBeginOverlap
  (params (OtherActor :type Actor%20Object%20Reference)))

(event EventTick
  (params (DeltaSeconds :type Float%20%28single-precision%29)))

(fn ConstructionScript)