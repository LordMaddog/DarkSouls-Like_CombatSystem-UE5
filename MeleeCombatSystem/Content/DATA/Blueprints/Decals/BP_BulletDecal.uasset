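; BP_BulletDecal is a bullet impact actor that leaves a fading decal and pushes nearby physics with a radial impulse.
; On BeginPlay it fires the impulse, snaps the decal onto the surface with a short forward sphere trace, then fades and destroys itself.
; A recursive Shrink event tapers smoke spawn rate but is not called here.
; Scorch-mark and hit-sound nodes are left unconnected.
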(event Custom|Shrink
  (Niagara|SetNiagaraVariable(Float) (Variables|Default|GetSmoke) "SpawnRate" (Variables|Default|GetSpawnRate))
  (Utilities|FlowControl|Delay 0.5)
  (bind _result (Math|Float|DecrementFloat (Variables|Default|GetSpawnRate))
    (:%20%20
      (if (> _result 0.0)
        (CallFunction|Shrink)))))

(event EventBeginPlay
  (Utilities|FlowControl|Delay 0.0)
  (Class|RadialForceComponent|FireImpulse (Variables|Default|GetRadialForce))
  (CallFunction|PlaceDecal)
  (Rendering|Components|Decal|SetFadeOut (Variables|Default|GetDecal) 0.1 4e+01 true)
  (Utilities|FlowControl|Delay 4e+01)
  (Actor|DestroyActor))

(fn ConstructionScript)

(fn PlaceDecal
  (bind _returnvalue (Transformation|GetActorLocation))
  (bind (_outhit _returnvalue_2) (Collision|SphereTraceByChannel _returnvalue (+ _returnvalue (* (Transformation|GetActorForwardVector) 2e+01)) 1.0 "TraceTypeQuery1" false 0 "None"))
  (if _returnvalue_2
    (Transformation|SetWorldLocation (Variables|Default|GetDecal) (.Location (Collision|BreakHitResult _outhit)) false false)))