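; XP drop pickup that homes toward the player and grants scaled experience on overlap or interact.
; Within range, or on PulltoPlayer, impulses push its cube toward the player; pull power grows periodically, and strong pull widens the pickup sphere.
; Collection fires once, playing particles and sound, adding stat-multiplied XP, showing the gain, then destroying itself.
; The construction script sizes the Niagara effect by XP value and switches larger drops to a green system.
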(event OnComponentBeginOverlap(Sphere)
  (params (OverlappedComponent :type Primitive%20Component%20Object%20Reference) (OtherActor :type Actor%20Object%20Reference) (OtherComp :type Primitive%20Component%20Object%20Reference) (OtherBodyIndex :type Integer) (bFromSweep :type Boolean) (SweepResult :type Hit%20Result%20Structure%20%28by%20ref%29))
  (bind _character (Variables|Default|GetCharacter))
  (bind _xpgiven (Variables|Default|GetXPGiven))
  (bind _character_2 (Variables|Default|GetCharacter))
  (bind _statscomponent (Variables|/Game/DATA/BP_PC.BP_PC_C|GetStatsComponent _character_2))
  (bind _statscomponent_2 (Variables|/Game/DATA/BP_PC.BP_PC_C|GetStatsComponent _character))
  (bind _value (Default|GetSubStats _statscomponent "NewEnumerator20"))
  (bind _returnvalue (* _xpgiven _value))
  (bind _returnvalue_2 (Math|Float|Truncate _returnvalue))
  ;[1 1 1] Give XP and delete self
  (if (== OtherActor (Game|GetPlayerCharacter 0))
    (Utilities|FlowControl|DoOnce false
      (:Completed
        (Components|Activation|Activate (Variables|Default|GetParticleSystem) true)
        (Utilities|FlowControl|Delay 0.1)
        (Utilities|IsValid _statscomponent_2
          (:Is%20Valid
            (Default|ModifyXP _statscomponent_2 "NewEnumerator0" _returnvalue_2)
            (Audio|PlaySoundatLocation "/Game/DATA/SoundFX/XP/SC_Xp.SC_Xp" (Transformation|GetActorLocation) "0, 0, 0" 1.0 1.0 0.0 0 0 0 0)
            (Default|DisplayGainedXP (Variables|/Game/DATA/BP_PC.BP_PC_C|GetInventory (Variables|Default|GetCharacter)) _returnvalue_2)
            (Actor|DestroyActor)))))))

(event EventBeginPlay
  ;[1 1 1] Start
  (|CallParentFunction)
  (bind _asbp_pc (Utilities|Casting|CastToBP_PC (Game|GetPlayerCharacter 0)))
  (Variables|Default|SetCharacter _asbp_pc)
  (Utilities|FlowControl|Delay 1e+01 :!label _label)
  (Math|Float|IncrementFloat (Variables|Default|GetPullPower)
    (:%20%20
      (goto _label))))

(event EventPulltoPlayer
  (params (Actor :type Vector :default "0, 0, 0") (PullPower :type Float%20%28double-precision%29))
  (bind _returnvalue (+ PullPower (Variables|Default|GetPullPower)))
  ;[1 1 1] Pull XP
  (Utilities|FlowControl|Sequence
    (:then_0
      (Physics|AddImpulse (Variables|Default|GetCube) (+ (* (Math|Vector|GetForwardVector (Math|Rotator|FindLookatRotation (Transformation|GetWorldLocation (Variables|Default|GetCube)) (Transformation|GetActorLocation (Variables|Default|GetCharacter)))) _returnvalue) "0.000000,0.000000,8.000000") "None" true))
    (:then_1
      (if (> _returnvalue 3e+02)
        (Components|Sphere|SetSphereRadius (Variables|Default|GetSphere) 2e+02 true)))))

(event EventTick
  (params (DeltaSeconds :type Float%20%28single-precision%29))
  ;[1 1 1] Pull XP
  (if (<= (Math|Vector|Distance(Vector) (Transformation|GetWorldLocation (Variables|Default|GetCube)) (Transformation|GetActorLocation (Variables|Default|GetCharacter))) 4e+02)
    (Utilities|FlowControl|Sequence
      (:then_0
        (Physics|AddImpulse (Variables|Default|GetCube) (+ (* (Math|Vector|GetForwardVector (Math|Rotator|FindLookatRotation (Transformation|GetWorldLocation (Variables|Default|GetCube)) (Transformation|GetActorLocation (Variables|Default|GetCharacter)))) (+ (stale EventPulltoPlayer PullPower) (Variables|Default|GetPullPower))) "0.000000,0.000000,8.000000") "None" true))
      (:then_1
        (if (> (+ (stale EventPulltoPlayer PullPower) (Variables|Default|GetPullPower)) 3e+02)
          (Components|Sphere|SetSphereRadius (Variables|Default|GetSphere) 2e+02 true))))))

(event EventInteract
  (params (CallEvent :type Actor%20Object%20Reference))
  (bind _character (Variables|Default|GetCharacter))
  (bind _xpgiven (Variables|Default|GetXPGiven))
  (bind _character_2 (Variables|Default|GetCharacter))
  (bind _statscomponent (Variables|/Game/DATA/BP_PC.BP_PC_C|GetStatsComponent _character_2))
  (bind _statscomponent_2 (Variables|/Game/DATA/BP_PC.BP_PC_C|GetStatsComponent _character))
  (bind _value (Default|GetSubStats _statscomponent "NewEnumerator20"))
  (bind _returnvalue (* _xpgiven _value))
  (bind _returnvalue_2 (Math|Float|Truncate _returnvalue))
  ;[1 1 1] Give XP and delete self
  (Utilities|FlowControl|DoOnce false
    (:Completed
      (Components|Activation|Activate (Variables|Default|GetParticleSystem) true)
      (Utilities|FlowControl|Delay 0.1)
      (Utilities|IsValid _statscomponent_2
        (:Is%20Valid
          (Default|ModifyXP _statscomponent_2 "NewEnumerator0" _returnvalue_2)
          (Audio|PlaySoundatLocation "/Game/DATA/SoundFX/XP/SC_Xp.SC_Xp" (Transformation|GetActorLocation) "0, 0, 0" 1.0 1.0 0.0 0 0 0 0)
          (Default|DisplayGainedXP (Variables|/Game/DATA/BP_PC.BP_PC_C|GetInventory (Variables|Default|GetCharacter)) _returnvalue_2)
          (Actor|DestroyActor))))))

(fn ConstructionScript
  (|CallParentFunction)
  (Effects|Components|ParticleSystem|SetFloatParameter (Variables|Default|GetN_Experience) "SpriteSize" (Math|Conversions|ToFloat(Integer) (+ (Variables|Default|GetXPGiven) 10)))
  (Effects|Components|ParticleSystem|SetFloatParameter (Variables|Default|GetN_Experience) "RibbonWidth" (+ (* (Variables|Default|GetXPGiven) 0.1) 2.0))
  (if (>= (Variables|Default|GetXPGiven) 20)
    (Class|NiagaraComponent|SetAsset (Variables|Default|GetN_Experience) "/Game/DATA/Effects/N_ExperienceParticelGreen.N_ExperienceParticelGreen" true)
    (Effects|Components|ParticleSystem|SetFloatParameter (Variables|Default|GetN_Experience) "SpriteSize" (+ (/ (Variables|Default|GetXPGiven) 10) 1e+01))
    (Effects|Components|ParticleSystem|SetFloatParameter (Variables|Default|GetN_Experience) "RibbonWidth" (+ (* (Variables|Default|GetXPGiven) 0.01) 2.0))))