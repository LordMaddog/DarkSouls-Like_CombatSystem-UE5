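; Placed spawner that creates one item pickup, picked by weighted chance from ItemsThatCanDrop.
; Construction script previews the first entry with a valid mesh, adding copies for stacked amounts.
; BeginPlay binds to the game instance's load-complete event; the spawn handler removes the preview and spawns unless its name is in the save's UsedItems.
; Spawning sets the amount, generates rarity for certain categories and records the spawner as used.
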(event Custom|LoadDoneSpawn
  (CallFunction|DestroyPreview)
  (if (== (Utilities|Array|FindItem (Variables|/Game/DATA/Blueprints/SaveGame/BP_SaveGame.BP_SaveGame_C|GetUsedItems (Variables|/Game/DATA/BP_Gameinstance.BP_Gameinstance_C|GetSaveGame (Variables|Default|GetGameinstance))) (Utilities|GetObjectName self)) -1)
    (bind _array_element (CallFunction|SelectItem))
    (bind _returnvalue (Game|SpawnActorfromClass _array_element (Transformation|GetActorTransform) "AdjustIfPossibleButAlwaysSpawn" "MultiplyWithRoot" self (Utilities|GetClassDefaults _array_element) "NewEnumerator2" (.amount (.Value (Utilities|Map|Find (Variables|Default|GetItemsThatCanDrop) _array_element))) "NewEnumerator7" "NewEnumerator0" 0 0 0 "NewEnumerator1" true 0))
    (CallFunction|GenerateRarity _returnvalue)
    (Utilities|Array|Add (Variables|/Game/DATA/Blueprints/SaveGame/BP_SaveGame.BP_SaveGame_C|GetUsedItems (Variables|/Game/DATA/BP_Gameinstance.BP_Gameinstance_C|GetSaveGame (Variables|Default|GetGameinstance))) (Utilities|GetObjectName self))))

(event EventBeginPlay
  (bind _asbp_gameinstance (Utilities|Casting|CastToBP_Gameinstance (Game|GetGameInstance)))
  (Variables|Default|SetGameinstance _asbp_gameinstance)
  (EventDispatchers|BindEventtoSendLoadComplete _asbp_gameinstance (EventDispatchers|CreateEvent :!event Custom|LoadDoneSpawn)))

(fn ConstructionScript
  (bind _displayitem (Variables|Default|GetDisplayItem))
  (bind _keys (Utilities|Map|Keys (Variables|Default|GetItemsThatCanDrop)))
  (bind _array_element (Utilities|Array|ForEachLoopwithBreak _keys :!label _label)
    (:LoopBody
      (Utilities|IsValid (.Mesh (Utilities|Struct|BreakS_StaticMeshTransform (.Static%20Mesh (Utilities|GetClassDefaults _array_element))))
        (:Is%20Valid
          (Components|StaticMesh|SetStaticMesh _displayitem (.Mesh (Utilities|Struct|BreakS_StaticMeshTransform (.Static%20Mesh (Utilities|GetClassDefaults _array_element)))))
          (Transformation|SetRelativeTransform _displayitem (.Loc (Utilities|Struct|BreakS_StaticMeshTransform (.Static%20Mesh (Utilities|GetClassDefaults _array_element)))) false false)
          (CallFunction|AddVisualItem (.ItemLoc (Utilities|GetClassDefaults _array_element)) (.amount (.Value (Utilities|Map|Find (Variables|Default|GetItemsThatCanDrop) _array_element))))
          (goto _label Break))))))

(fn GenerateRarity
  (params (Target :type BP%20Master%20Item%20Object%20Reference))
  (bind _iteminfo (Variables|/Game/DATA/Blueprints/Actors/BP_MasterItem.BP_MasterItem_C|GetItemInfo Target))
  (bind _category (Utilities|Struct|BreakS_ItemInfo _iteminfo))
  (if (Utilities|Enum|Equal(Enum) _category "NewEnumerator0")
    (Default|GenerateRarity Target 0.0 :!label _label)
    (elif (Utilities|Enum|Equal(Enum) _category "NewEnumerator2")
      (goto _label))))

(fn SelectItem
  (bind _keys (Utilities|Map|Keys (Variables|Default|GetItemsThatCanDrop)))
  (for _array_element _keys
    (LocalVariables|SetMax (+ (LocalVariables|GetMax) (.chance (.Value (Utilities|Map|Find (Variables|Default|GetItemsThatCanDrop) _array_element))))))
  (LocalVariables|SetRandomNumber (Math|Random|RandomFloatinRange 0.0 (LocalVariables|GetMax)))
  (bind _keys_2 (Utilities|Map|Keys (Variables|Default|GetItemsThatCanDrop)))
  (for _array_element_2 _keys_2
    (bind _output_get (LocalVariables|SetCurrent (+ (.chance (.Value (Utilities|Map|Find (Variables|Default|GetItemsThatCanDrop) _array_element_2))) (LocalVariables|GetCurrent))))
    (if (>= _output_get (LocalVariables|GetRandomNumber))
      (return _array_element_2))))

(fn AddVisualItem
  (params (Item%20Loc :type Array%20of%20Transforms) (Amount :type Integer))
  (bind _displayitem (Variables|Default|GetDisplayItem))
  (if (not (Variables|Default|GetGenerated))
    (Variables|Default|SetGenerated true)
    (if (> Amount 1)
      (for _array_element Item%20Loc
        (if (> Amount (LocalVariables|GetSpawnCount))
          (Math|Integer|IncrementInt (LocalVariables|GetSpawnCount)
            (:%20%20
              (bind _returnvalue (AddComponent|AddStaticMeshComponent false (Math|Transform|MakeTransform (.Location (Math|Transform|BreakTransform _array_element)) (.Rotation (Math|Transform|BreakTransform _array_element)) (.Scale (Math|Transform|BreakTransform _array_element)))))
              (Components|StaticMesh|SetStaticMesh _returnvalue (Variables|/Script/Engine.StaticMeshComponent|GetStaticMesh _displayitem))
              (Rendering|Material|SetMaterial _returnvalue 0 (Rendering|Material|GetMaterial _displayitem 0))
              (Transformation|AttachComponentToComponent _returnvalue _displayitem "None" "KeepWorld" "KeepWorld" "KeepWorld" true)
              (Utilities|Array|Add (Variables|Default|GetDisplayedItems) _returnvalue))))))))

(fn DestroyPreview
  (Utilities|IsValid (Variables|Default|GetDisplayItem)
    (:Is%20Valid
      (Components|DestroyComponent (Variables|Default|GetDisplayItem))
      (for _array_element (Variables|Default|GetDisplayedItems)
        (Components|DestroyComponent _array_element)))))