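; BP_ShatteredBlade is a child armor Blueprint that adds an NShatteredBlade component to the parent's equip behavior.
; On equip, SetRandomLoc teleports that component to a random relative Y and Z offset, keeping its X.
; Removing the equip mesh runs the parent logic, then destroys the component if it is still valid.
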(event EventBeginPlay
  (|CallParentFunction))

(event Collision|EventActorBeginOverlap
  (params (OtherActor :type Actor%20Object%20Reference))
  (|CallParentFunction OtherActor) ; This node is disabled and will not be called.\nDrag off pins to build functionality.
)

(event EventTick
  (params (DeltaSeconds :type Float%20%28single-precision%29))
  (|CallParentFunction DeltaSeconds))

(fn ConstructionScript
  (|CallParentFunction))

(fn RemoveEquipMesh
  (bind _n_shatteredblade (Variables|Default|GetN_shatteredBlade))
  (|CallParentFunction)
  (Utilities|IsValid _n_shatteredblade
    (:Is%20Valid
      (Components|DestroyComponent _n_shatteredblade))))

(fn OnEquipped
  (|CallParentFunction)
  (CallFunction|SetRandomLoc (Variables|Default|GetN_shatteredBlade)))

(fn SetRandomLoc
  (params (Target :type Scene%20Component%20Object%20Reference))
  (Transformation|SetRelativeLocation Target (Math|Vector|MakeVector (.x (Variables|/Script/Engine.SceneComponent|GetRelativeLocation Target)) (Math|Random|RandomFloatinRange -3e+01 2e+02) (Math|Random|RandomFloatinRange -3e+01 2e+02)) false true))