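; Stone status effect built as an equippable item that petrifies the character it is equipped on.
; Equipping attaches an earth Niagara effect to the mesh, plays a sound and runs a timeline easing custom time dilation to zero, then applies a rock overlay material.
; NPCs then repeatedly play louder effort sounds while draining an element stat to break out.
; Unequipping plays a break sound, restores time and material, and changes the NPC's maximum of that element.
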(event Custom|ApplyEffect
  (bind _equipped_character (Variables|Default|GetEquipped%20Character))
  (bind _mesh (Variables|/Script/Engine.Character|GetMesh _equipped_character))
  ;[1 1 1] Apply Effect
  (bind _returnvalue (Niagara|SpawnSystemAttached "/Game/DATA/Effects/N_Earth_Body.N_Earth_Body" _mesh "None" (Transformation|GetWorldLocation _mesh) "0, 0, 0" "KeepRelativeOffset" true))
  (bind _output_get (Variables|Default|SetEffect _returnvalue))
  (Class|NiagaraFunctionLibrary|OverrideSystemUserVariableSkeletalMeshComponent _output_get "SkeletalMesh" (Variables|/Script/Engine.Character|GetMesh (Variables|Default|GetEquipped%20Character)))
  (Components|Activation|Activate (Variables|Default|GetPetrifycationSound) true)
  (bind _alpha (Timeline|Petrify PlayFromStart)
    (:Update
      (Variables|/Script/Engine.Actor|SetCustomTimeDilation (Variables|Default|GetEquipped%20Character) (Math|Float|Lerp 1.0 0.0 _alpha)))
    (:Finished
      (Rendering|Material|SetOverlayMaterial (Variables|/Script/Engine.Character|GetMesh (Variables|Default|GetEquipped%20Character)) "/Game/InfinityBladeIceLands/Environments/Ice/Ice_Castle/Materials/EX_Env_Rock_Icy_D_Mat.EX_Env_Rock_Icy_D_Mat" :!class /Script/Engine.MeshComponent)
      (if (not (Variables|/Game/DATA/Blueprints/Components/CombatComponent.CombatComponent_C|GetIsPlayer (Variables|/Game/DATA/BP_PC.BP_PC_C|GetCombatComponent (Variables|Default|GetEquipped%20Character))))
        (Utilities|Time|SetTimerbyFunctionName 0 "NPCBrakeOut" 0.5 true)))))

(event Custom|RemoveEffect
  ;[1 1 1] Remove Effect
  (Audio|Components|Audio|SetSound (Variables|Default|GetPetrifycationSound) "/Game/DATA/SoundFX/Earth/BuildingRumble/SC_StoneBrake.SC_StoneBrake")
  (Components|Activation|Activate (Variables|Default|GetPetrifycationSound) true)
  (Components|Activation|Deactivate (Variables|Default|GetEffect))
  (Variables|/Script/Engine.Actor|SetCustomTimeDilation (Variables|Default|GetEquipped%20Character) 1.0)
  (Rendering|Material|SetOverlayMaterial (Variables|/Script/Engine.Character|GetMesh (Variables|Default|GetEquipped%20Character)) 0 :!class /Script/Engine.MeshComponent)
  (if (not (Variables|/Game/DATA/Blueprints/Components/CombatComponent.CombatComponent_C|GetIsPlayer (Variables|/Game/DATA/BP_PC.BP_PC_C|GetCombatComponent (Variables|Default|GetEquipped%20Character))))
    (Default|ModifyMaxElement (Variables|/Game/DATA/BP_PC.BP_PC_C|GetStatsComponent (Variables|Default|GetEquipped%20Character)) "NewEnumerator4" 1e+02)))

(event Custom|NPCBrakeOut
  (bind _equipped_character (Variables|Default|GetEquipped%20Character))
  (bind _combatcomponent (Variables|/Game/DATA/BP_PC.BP_PC_C|GetCombatComponent _equipped_character))
  ;[1 1 1] NPC Brake out
  (if (not (Variables|/Game/DATA/Blueprints/Components/CombatComponent.CombatComponent_C|GetDead (Variables|/Game/DATA/BP_PC.BP_PC_C|GetCombatComponent (Variables|Default|GetEquipped%20Character))))
    (Default|PlayVoiceSoundVolume _combatcomponent (Variables|/Game/DATA/Blueprints/Components/CombatComponent.CombatComponent_C|GetAttackEffortSound _combatcomponent) (Variables|Default|GetVolume))
    (Variables|Default|SetVolume (Math|Float|Clamp(Float) (+ (Variables|Default|GetVolume) 0.2) (+ (Variables|Default|GetVolume) 0.2)))
    (Default|ModifyCurrentElement (Variables|/Game/DATA/BP_PC.BP_PC_C|GetStatsComponent (Variables|Default|GetEquipped%20Character)) "NewEnumerator4" -25.0)))

(event EventBeginPlay
  (|CallParentFunction) ; This node is disabled and will not be called.\nDrag off pins to build functionality.
)

(event Collision|EventActorBeginOverlap
  (params (OtherActor :type Actor%20Object%20Reference))
  (|CallParentFunction OtherActor) ; This node is disabled and will not be called.\nDrag off pins to build functionality.
)

(event EventTick
  (params (DeltaSeconds :type Float%20%28single-precision%29))
  (|CallParentFunction DeltaSeconds) ; This node is disabled and will not be called.\nDrag off pins to build functionality.
)

(fn ConstructionScript
  (|CallParentFunction))

(fn OnEquipped
  (|CallParentFunction)
  (CallFunction|ApplyEffect))

(fn OnUnequipped
  (params (GiveBack? :type Boolean) (ForceDrop :type Boolean) (ItemInfoIn :type S%20Item%20Info%20Structure))
  (CallFunction|RemoveEffect)
  (|CallParentFunction GiveBack? ForceDrop ItemInfoIn))