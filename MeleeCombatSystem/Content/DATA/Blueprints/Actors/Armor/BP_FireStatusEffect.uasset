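; Fire status effect built as an equippable armor actor that burns its wearer while equipped.
; Equipping calls ApplySpeedDown, which, despite its name, attaches body-fire Niagara to the character mesh, plays sounds and starts a looping BurnDamage timer.
; Each second it deals magic point damage proportional to a max stat, using a sphere trace only for hit info.
; Unequipping deactivates the particles but never clears the timer.
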(event Custom|ApplySpeedDown
  (bind _equipped_character (Variables|Default|GetEquipped%20Character))
  (bind _mesh (Variables|/Script/Engine.Character|GetMesh _equipped_character))
  (bind _returnvalue (Niagara|SpawnSystemAttached "/Game/DATA/Effects/N_Fire_Body.N_Fire_Body" _mesh "None" (Transformation|GetWorldLocation _mesh) "0, 0, 0" "KeepRelativeOffset" true))
  (bind _output_get (Variables|Default|SetEffect _returnvalue))
  (Class|NiagaraFunctionLibrary|OverrideSystemUserVariableSkeletalMeshComponent _output_get "SkeletalMesh" (Variables|/Script/Engine.Character|GetMesh (Variables|Default|GetEquipped%20Character)))
  (Utilities|Time|SetTimerbyFunctionName 0 "BurnDamage" 1.0 true)
  (Audio|PlaySoundatLocation "/Game/DATA/SoundFX/Fire/SC_FireGenaric_1.SC_FireGenaric_1" (Transformation|GetWorldLocation (Variables|/Script/Engine.Character|GetMesh (Variables|Default|GetEquipped%20Character))) "0, 0, 0" 1.0 1.0 0.0 0 0 0 0)
  (Audio|PlaySoundatLocation "/Game/DATA/SoundFX/Fire/SC_FireGeneric_2.SC_FireGeneric_2" (Transformation|GetWorldLocation (Variables|/Script/Engine.Character|GetMesh (Variables|Default|GetEquipped%20Character))) "0, 0, 0" 1.0 1.0 0.0 0 0 0 0))

(event Custom|RemoveEffect
  (Components|Activation|Deactivate (Variables|Default|GetEffect)))

(event Custom|BurnDamage
  (bind _equipped_character (Variables|Default|GetEquipped%20Character))
  (bind _equipped_character_2 (Variables|Default|GetEquipped%20Character))
  (bind _returnvalue (Transformation|GetActorLocation _equipped_character_2))
  (Audio|PlaySoundatLocation "/Game/DATA/SoundFX/Fire/SC_FireGeneric_2.SC_FireGeneric_2" (Transformation|GetWorldLocation (Variables|/Script/Engine.Character|GetMesh (Variables|Default|GetEquipped%20Character))) "0, 0, 0" 1.0 1.0 0.0 0 0 0 0)
  (Utilities|FlowControl|Delay 0.2)
  (bind _outhit (Collision|SphereTraceForObjects _returnvalue _returnvalue 1e+01 (Utilities|Array|MakeArray "ObjectTypeQuery3") false (Utilities|Array|MakeArray self _equipped_character_2) "None"))
  (Game|Damage|ApplyPointDamage (Variables|Default|GetEquipped%20Character) (* (Default|GetMaxStatValue (Variables|/Game/DATA/BP_PC.BP_PC_C|GetStatsComponent _equipped_character) "NewEnumerator1") 0.1) (.Location (Collision|BreakHitResult _outhit)) _outhit 0 _equipped_character "/Game/DATA/Blueprints/DamageTypes/BP_AttackDamageType_Magic.BP_AttackDamageType_Magic_C"))

(event EventBeginPlay
  (|CallParentFunction) ; This node is disabled and will not be called.\nDrag off pins to build functionality.
)

(event Collision|EventActorBeginOverlap
  (params (OtherActor :type Actor%20Object%20Reference))
  (|CallParentFunction OtherActor) ; This node is disabled and will not be called.\nDrag off pins to build functionality.
)

(event EventTick
  (params (DeltaSeconds :type Float%20%28single-precision%29))
  (|CallParentFunction DeltaSeconds) ; This node is disabled and will not be called.\nDrag off pins to build functionality.
)

(fn ConstructionScript
  (|CallParentFunction))

(fn OnEquipped
  (|CallParentFunction)
  (CallFunction|ApplySpeedDown))

(fn OnUnequipped
  (params (GiveBack? :type Boolean) (ForceDrop :type Boolean) (ItemInfoIn :type S%20Item%20Info%20Structure))
  (CallFunction|RemoveEffect)
  (|CallParentFunction GiveBack? ForceDrop ItemInfoIn))