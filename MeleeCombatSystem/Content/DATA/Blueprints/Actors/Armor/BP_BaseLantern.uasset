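; Base lantern item Blueprint, filed with armor actors, that adjusts its mesh and light components when equipped or dropped.
; GetRelitive caches the item mesh's relative transform, though nothing in this Blueprint calls it.
; OnEquipped runs parent logic, destroys Light1 and reapplies that cached transform to the mesh.
; OnDropped runs parent logic, then destroys the Light and PointLight components if they are valid.
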(event Custom|GetRelitive
  (Variables|Default|SetTransform (Transformation|GetRelativeTransform (Variables|Default|GetItemStaticMesh))))

(event EventBeginPlay
  (|CallParentFunction) ; This node is disabled and will not be called.\nDrag off pins to build functionality.
)

(event Collision|EventActorBeginOverlap
  (params (OtherActor :type Actor%20Object%20Reference))
  (|CallParentFunction OtherActor) ; This node is disabled and will not be called.\nDrag off pins to build functionality.
)

(event EventTick
  (params (DeltaSeconds :type Float%20%28single-precision%29))
  (|CallParentFunction DeltaSeconds) ; This node is disabled and will not be called.\nDrag off pins to build functionality.
)

(event EventOnDropped
  (bind _light (Variables|Default|GetLight))
  (bind _pointlight (Variables|Default|GetPointLight))
  (|CallParentFunction)
  (Utilities|FlowControl|Sequence
    (:then_0
      (Utilities|IsValid _light
        (:Is%20Valid
          (Components|DestroyComponent _light))))
    (:then_1
      (Utilities|IsValid _pointlight
        (:Is%20Valid
          (Components|DestroyComponent _pointlight))))))

(fn ConstructionScript
  (|CallParentFunction))

(fn OnEquipped
  (|CallParentFunction)
  (Components|DestroyComponent (Variables|Default|GetLight1))
  (Transformation|SetRelativeTransform (Variables|Default|GetItemStaticMesh) (Variables|Default|GetTransform) false false))