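; Wind status effect, built as an equippable actor, that knocks its equipped character off their feet.
; On equip it attaches a Niagara wind effect to the mesh, plays a sound, then ragdolls the character with a randomly offset radial impulse from below.
; A second later it drains one of the character's element stats; unequipping deactivates the effect.
; The stamina-damage and random hit-reaction event is present, but its looping timer is disconnected.
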(event Custom|ApplyEffect
  (bind _returnvalue (Math|Random|RandomFloatinRange -5e+01 5e+01))
  (bind _equipped_character (Variables|Default|GetEquipped%20Character))
  (bind _equipped_character_2 (Variables|Default|GetEquipped%20Character))
  (bind _statscomponent (Variables|/Game/DATA/BP_PC.BP_PC_C|GetStatsComponent _equipped_character))
  (bind _mesh (Variables|/Script/Engine.Character|GetMesh _equipped_character_2))
  (bind _returnvalue_2 (Niagara|SpawnSystemAttached "/Game/DATA/Effects/N_Wind_Body.N_Wind_Body" _mesh "None" (Transformation|GetWorldLocation _mesh) "0, 0, 0" "KeepRelativeOffset" true))
  (bind _output_get (Variables|Default|SetEffect _returnvalue_2))
  (Class|NiagaraFunctionLibrary|OverrideSystemUserVariableSkeletalMeshComponent _output_get "SkeletalMesh" (Variables|/Script/Engine.Character|GetMesh (Variables|Default|GetEquipped%20Character)))
  (Audio|PlaySoundatLocation "/Game/DATA/SoundFX/Wind/SC_WindGeneric_1.SC_WindGeneric_1" (Transformation|GetWorldLocation (Variables|/Script/Engine.Character|GetMesh (Variables|Default|GetEquipped%20Character))) "0, 0, 0" 1.0 1.0 0.0 0 0 0 0)
  (Utilities|FlowControl|Delay 0.2)
  (Default|EnableRagdoll (Variables|/Game/DATA/BP_PC.BP_PC_C|GetCombatComponent (Variables|Default|GetEquipped%20Character)))
  (Physics|AddRadialImpulse (Variables|/Script/Engine.Character|GetMesh (Variables|Default|GetEquipped%20Character)) (+ (Transformation|GetActorLocation (Variables|Default|GetEquipped%20Character)) (Math|Vector|MakeVector _returnvalue _returnvalue -5e+01)) 1e+02 1e+03 "RIF_Constant" true)
  (Utilities|FlowControl|Delay 1.0)
  (Default|ModifyCurrentElement _statscomponent "NewEnumerator5" (* (Default|GetMaxElement _statscomponent "NewEnumerator5") -1.1)))

(event Custom|RemoveEffect
  (Components|Activation|Deactivate (Variables|Default|GetEffect)))

(event Custom|StamDamage
  (bind _equipped_character (Variables|Default|GetEquipped%20Character))
  (bind _statscomponent (Variables|/Game/DATA/BP_PC.BP_PC_C|GetStatsComponent _equipped_character))
  (Default|ModifyCurrentStatValue _statscomponent "NewEnumerator2" (* (* (Default|GetMaxStatValue _statscomponent "NewEnumerator2") 0.2) -1.0) true)
  (if (> (Math|Random|RandomFloatinRange 1.0 1e+02) 7e+01)
    (Default|PerformHitReactionManual (Variables|/Game/DATA/BP_PC.BP_PC_C|GetCombatComponent (Variables|Default|GetEquipped%20Character)) (Utilities|Enum|ByteToEnumE_HitDirection (Math|Conversions|ToByte(Integer) (Math|Random|RandomIntegerinRange 0 3))) "NewEnumerator1")))

(event EventBeginPlay
  (|CallParentFunction) ; This node is disabled and will not be called.\nDrag off pins to build functionality.
)

(event Collision|EventActorBeginOverlap
  (params (OtherActor :type Actor%20Object%20Reference))
  (|CallParentFunction OtherActor) ; This node is disabled and will not be called.\nDrag off pins to build functionality.
)

(event EventTick
  (params (DeltaSeconds :type Float%20%28single-precision%29))
  (|CallParentFunction DeltaSeconds) ; This node is disabled and will not be called.\nDrag off pins to build functionality.
)

(fn ConstructionScript
  (|CallParentFunction))

(fn OnEquipped
  (|CallParentFunction)
  (CallFunction|ApplyEffect))

(fn OnUnequipped
  (params (GiveBack? :type Boolean) (ForceDrop :type Boolean) (ItemInfoIn :type S%20Item%20Info%20Structure))
  (CallFunction|RemoveEffect)
  (|CallParentFunction GiveBack? ForceDrop ItemInfoIn))