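; BP_EhudsDagger is equippable gear that shows a Niagara dagger and automatically attacks other living player characters near its wearer.
; A Guard loop waits a random interval, picks a target in its sphere, sphere-traces for line of sight, then spawns BP_SpellEhudsDagger and hides the dagger.
; A Niagara particle export callback supplies the launch position, while Tick steers particle facing.
; ArtifactSpellDone restores visibility and either restarts guarding or recasts.
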(event Custom|Guard
  (bind _equipped_character (Variables|Default|GetEquipped%20Character))
  (Utilities|FlowControl|Delay (Math|Random|RandomFloatinRange 2.0 6.0))
  (for _array_element (Collision|GetOverlappingActors (Variables|Default|GetSphereAttackRadius) "/Game/DATA/BP_PC.BP_PC_C" :!class /Script/Engine.PrimitiveComponent)
    (if (!= _array_element (Variables|Default|GetEquipped%20Character))
      (bind _asbp_pc (Utilities|Casting|CastToBP_PC _array_element))
      (if (not (Variables|/Game/DATA/Blueprints/Components/CombatComponent.CombatComponent_C|GetDead (Variables|/Game/DATA/BP_PC.BP_PC_C|GetCombatComponent _asbp_pc)))
        (Variables|Default|SetTarget _asbp_pc)
        (Variables|Default|SetTarget%20Selected true))))
  (Utilities|FlowControl|Delay 1.0)
  (Variables|Default|SetTarget%20Selected false)
  (Utilities|IsValid (Variables|Default|GetTarget)
    (:Is%20Valid
      (bind _outhit (Collision|SphereTraceForObjects (Variables|Default|GetPartical%20location) (Transformation|GetActorLocation (Variables|Default|GetTarget)) 15.0 (Utilities|Array|MakeArray "ObjectTypeQuery1" "ObjectTypeQuery9" "ObjectTypeQuery6" "ObjectTypeQuery8") false 0 "None"))
      (if (== (.HitActor (Collision|BreakHitResult _outhit)) (Variables|Default|GetTarget))
        (Game|SpawnActorfromClass :Class "/Game/DATA/Blueprints/Actors/Magic/BP_SpellEhudsDagger.BP_SpellEhudsDagger_C" :SpawnTransform (Math|Transform|MakeTransform (Variables|Default|GetPartical%20location) (Math|Rotator|FindLookatRotation (Variables|Default|GetPartical%20location) (Transformation|GetActorLocation (Variables|Default|GetTarget))) "1.000000,1.000000,1.000000") :CollisionHandlingOverride "Undefined" :TransformScaleMethod "MultiplyWithRoot" :Owner _equipped_character :Target (Variables|Default|GetTarget) :Spawner self :MaxRange 6e+03 :Initial%20Speed 5e+02 :Character _equipped_character :FriendlyFire? false :Instigator _equipped_character)
        (Audio|SpawnSoundatLocation "/Game/DATA/SoundFX/Weapon/Sword/SC_Sword_Hit_Holow.SC_Sword_Hit_Holow" (Variables|Default|GetPartical%20location) "0, 0, 0" 1.0 1.0 0.0 0 0)
        (Rendering|SetVisibility (Variables|Default|GetN_EhudsDagger) false false)
        (else
          (CallFunction|Guard))))
    (:Is%20Not%20Valid
      (CallFunction|Guard))))

(event Custom|ReCast
  (bind _equipped_character (Variables|Default|GetEquipped%20Character))
  (for _array_element (Collision|GetOverlappingActors (Variables|Default|GetSphereAttackRadius) "/Game/DATA/BP_PC.BP_PC_C" :!class /Script/Engine.PrimitiveComponent)
    (if (!= _array_element (Variables|Default|GetEquipped%20Character))
      (bind _asbp_pc (Utilities|Casting|CastToBP_PC _array_element))
      (if (not (Variables|/Game/DATA/Blueprints/Components/CombatComponent.CombatComponent_C|GetDead (Variables|/Game/DATA/BP_PC.BP_PC_C|GetCombatComponent _asbp_pc)))
        (Variables|Default|SetTarget _asbp_pc)
        (Variables|Default|SetTarget%20Selected true))))
  (Utilities|FlowControl|Delay 1.0)
  (Variables|Default|SetTarget%20Selected false)
  (Utilities|IsValid (Variables|Default|GetTarget)
    (:Is%20Valid
      (bind _outhit (Collision|SphereTraceForObjects (Variables|Default|GetPartical%20location) (Transformation|GetActorLocation (Variables|Default|GetTarget)) 15.0 (Utilities|Array|MakeArray "ObjectTypeQuery1" "ObjectTypeQuery9" "ObjectTypeQuery6" "ObjectTypeQuery8") false 0 "None"))
      (if (== (.HitActor (Collision|BreakHitResult _outhit)) (Variables|Default|GetTarget))
        (Game|SpawnActorfromClass :Class "/Game/DATA/Blueprints/Actors/Magic/BP_SpellEhudsDagger.BP_SpellEhudsDagger_C" :SpawnTransform (Math|Transform|MakeTransform (Variables|Default|GetPartical%20location) (Math|Rotator|FindLookatRotation (Variables|Default|GetPartical%20location) (Transformation|GetActorLocation (Variables|Default|GetTarget))) "1.000000,1.000000,1.000000") :CollisionHandlingOverride "Undefined" :TransformScaleMethod "MultiplyWithRoot" :Owner _equipped_character :Target (Variables|Default|GetTarget) :Spawner self :MaxRange 6e+03 :Initial%20Speed 5e+02 :Character _equipped_character :FriendlyFire? false :Instigator _equipped_character)
        (Audio|SpawnSoundatLocation "/Game/DATA/SoundFX/Weapon/Sword/SC_Sword_Hit_Holow.SC_Sword_Hit_Holow" (Variables|Default|GetPartical%20location) "0, 0, 0" 1.0 1.0 0.0 0 0)
        (Rendering|SetVisibility (Variables|Default|GetN_EhudsDagger) false false)
        (else
          (CallFunction|Guard))))
    (:Is%20Not%20Valid
      (CallFunction|Guard))))

(event EventBeginPlay
  (|CallParentFunction))

(event Collision|EventActorBeginOverlap
  (params (OtherActor :type Actor%20Object%20Reference))
  (|CallParentFunction OtherActor) ; This node is disabled and will not be called.\nDrag off pins to build functionality.
)

(event EventTick
  (params (DeltaSeconds :type Float%20%28single-precision%29))
  (|CallParentFunction DeltaSeconds)
  (Utilities|IsValid (Variables|Default|GetN_EhudsDagger)
    (:Is%20Valid
      (if (not (Variables|Default|GetTarget%20Selected))
        (Effects|Components|ParticleSystem|SetVectorParameter (Variables|Default|GetN_EhudsDagger) "FacingDirection" (Math|Vector|GetForwardVector (Variables|/Game/DATA/BP_PC.BP_PC_C|GetVoice (Variables|Default|GetEquipped%20Character))) :!label _label)
        (else
          (Utilities|IsValid (Variables|Default|GetTarget)
            (:Is%20Valid
              (Effects|Components|ParticleSystem|SetVectorParameter (Variables|Default|GetN_EhudsDagger) "FacingDirection" (Math|Vector|GetForwardVector (Math|Rotator|FindLookatRotation (Variables|Default|GetPartical%20location) (Transformation|GetActorLocation (Variables|Default|GetTarget))))))
            (:Is%20Not%20Valid
              (goto _label))))))))

(event EventParticleData
  (params (Data :type Array%20of%20Basic%20Particle%20Data%20Structures) (NiagaraSystem :type Niagara%20System%20Object%20Reference) (SimulationPositionOffset :type Vector%20%28by%20ref%29 :default "0, 0, 0"))
  (for (_array_element _array_index) Data
    (if (== _array_index 0)
      (Variables|Default|SetPartical%20location (.position _array_element)))))

(event EventArtifactSpellDone
  (params (Index :type Integer))
  (if (< Index 1)
    (CallFunction|Guard)
    (else
      (CallFunction|ReCast)))
  (Rendering|SetVisibility (Variables|Default|GetN_EhudsDagger) true false))

(fn ConstructionScript
  (|CallParentFunction))

(fn RemoveEquipMesh
  (bind _n_ehudsdagger (Variables|Default|GetN_EhudsDagger))
  (|CallParentFunction)
  (Utilities|IsValid _n_ehudsdagger
    (:Is%20Valid
      (Components|DestroyComponent _n_ehudsdagger))))

(fn OnEquipped
  (Variables|Default|SetEquipType (Variables|Default|GetDesiredEquipType))
  (|CallParentFunction)
  (CallFunction|Guard)
  (Class|NiagaraComponent|SetVariableObject (Variables|Default|GetN_EhudsDagger) "BP_Postion" self))

(fn ParticalLoc
  (bind _returnvalue (Class|NiagaraDataInterfaceArrayFunctionLibrary|GetNiagaraArrayPosition (Variables|Default|GetN_EhudsDagger) "None"))
  (for (_array_element _array_index) _returnvalue
    (if (== _array_index 0)
      (Variables|Default|SetPartical%20location _array_element))))

(fn SetRandomLoc
  (params (Target :type Scene%20Component%20Object%20Reference))
  (Transformation|SetRelativeLocation Target (Math|Vector|MakeVector (.x (Variables|/Script/Engine.SceneComponent|GetRelativeLocation Target)) (Math|Random|RandomFloatinRange -5e+01 -1e+02) (Math|Random|RandomFloatinRange -5e+01 -1e+02)) false true))

(fn CanReciveDamage
  (return false))

(fn DamageType
  (return "NewEnumerator0"))

(fn GetCharacterInfo
  (return 0))

(fn GetDesiredRotation
  (return "0, 0, 0"))

(fn PreformCombatAction
  (params (ActionTag :type Gameplay%20Tag%20Structure) (SateTag :type Gameplay%20Tag%20Structure) (MontageIndex :type Integer) (bRandomItemIndex :type Boolean))
  (return 0.0))

(fn PreformCombatAttack
  (params (AttackType :type Gameplay%20Tag%20Structure) (SetState :type Gameplay%20Tag%20Structure) (AttackIndex :type Integer) (bRandomIndex :type Boolean))
  (return 0.0))

(fn PreformCustomAction
  (params (ActionTag :type Gameplay%20Tag%20Structure) (StateTag :type Gameplay%20Tag%20Structure) (InMontage :type Anim%20Montage%20Object%20Reference) (MontagePlayRate :type Float%20%28double-precision%29) (bAutoReset :type Boolean))
  (return false))

(fn UpdateMotionWarp
  (params (Name :type Name :default "None") (LOC :type Transform))
  (return "0, 0, 0"))