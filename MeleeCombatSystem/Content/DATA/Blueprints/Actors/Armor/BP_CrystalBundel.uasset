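; Equippable crystal bundle armor whose floating Niagara crystal automatically fires at nearby player characters.
; On equip, it randomly offsets the crystal and starts a self-repeating Guard loop with random delays, selecting living BP_PC actors other than the wearer within SphereAttackRadius.
; The Niagara system exports its particle position to the Blueprint as the origin for a line-of-sight sphere trace and the BP_SpellCrystalT1 projectile.
; Removing the equipment destroys the crystal.
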(event Custom|Guard
  (bind _equipped_character (Variables|Default|GetEquipped%20Character))
  (Utilities|FlowControl|Delay (Math|Random|RandomFloatinRange 2.0 6.0))
  (for _array_element (Collision|GetOverlappingActors (Variables|Default|GetSphereAttackRadius) "/Game/DATA/BP_PC.BP_PC_C" :!class /Script/Engine.PrimitiveComponent)
    (if (!= _array_element (Variables|Default|GetEquipped%20Character))
      (if (not (Variables|/Game/DATA/Blueprints/Components/CombatComponent.CombatComponent_C|GetDead (Actor|GetComponentbyClass _array_element "/Game/DATA/Blueprints/Components/CombatComponent.CombatComponent_C")))
        (Variables|Default|SetTarget _array_element))))
  (CallFunction|Guard)
  (Utilities|IsValid (Variables|Default|GetTarget)
    (:Is%20Valid
      (bind _outhit (Collision|SphereTraceForObjects (Variables|Default|GetPartical%20location) (Transformation|GetActorLocation (Variables|Default|GetTarget)) 15.0 (Utilities|Array|MakeArray "ObjectTypeQuery1" "ObjectTypeQuery9" "ObjectTypeQuery6" "ObjectTypeQuery8") false 0 "None"))
      (if (== (.HitActor (Collision|BreakHitResult _outhit)) (Variables|Default|GetTarget))
        (Game|SpawnActorfromClass :Class "/Game/DATA/Blueprints/Actors/Magic/BP_SpellCrystalT1.BP_SpellCrystalT1_C" :SpawnTransform (Math|Transform|MakeTransform (Variables|Default|GetPartical%20location) (Math|Rotator|FindLookatRotation (Variables|Default|GetPartical%20location) (Transformation|GetActorLocation (Variables|Default|GetTarget))) "1.000000,1.000000,1.000000") :CollisionHandlingOverride "Undefined" :TransformScaleMethod "MultiplyWithRoot" :Owner _equipped_character :MaxRange 6e+03 :Character _equipped_character :FriendlyFire? false :Instigator _equipped_character)
        (Audio|SpawnSoundatLocation "/Game/DATA/Meshes/BulletHeavenMagicItems/CrystalBundel/SC_CrystalCast.SC_CrystalCast" (Variables|Default|GetPartical%20location) "0, 0, 0" 1.0 1.0 0.0 0 0)))))

(event EventBeginPlay
  (|CallParentFunction))

(event Collision|EventActorBeginOverlap
  (params (OtherActor :type Actor%20Object%20Reference))
  (|CallParentFunction OtherActor) ; This node is disabled and will not be called.\nDrag off pins to build functionality.
)

(event EventTick
  (params (DeltaSeconds :type Float%20%28single-precision%29))
  (|CallParentFunction DeltaSeconds))

(event EventParticleData
  (params (Data :type Array%20of%20Basic%20Particle%20Data%20Structures) (NiagaraSystem :type Niagara%20System%20Object%20Reference) (SimulationPositionOffset :type Vector%20%28by%20ref%29 :default "0, 0, 0"))
  (for (_array_element _array_index) Data
    (if (== _array_index 0)
      (Variables|Default|SetPartical%20location (.position _array_element)))))

(fn ConstructionScript
  (|CallParentFunction))

(fn RemoveEquipMesh
  (bind _n_floatingcrystal (Variables|Default|GetN_FloatingCrystal))
  (|CallParentFunction)
  (Utilities|IsValid _n_floatingcrystal
    (:Is%20Valid
      (Components|DestroyComponent _n_floatingcrystal))))

(fn OnEquipped
  (|CallParentFunction)
  (CallFunction|Guard)
  (Class|NiagaraComponent|SetVariableObject (Variables|Default|GetN_FloatingCrystal) "BP_Postion" self)
  (CallFunction|SetRandomLoc (Variables|Default|GetN_FloatingCrystal)))

(fn ParticalLoc
  (bind _returnvalue (Class|NiagaraDataInterfaceArrayFunctionLibrary|GetNiagaraArrayPosition (Variables|Default|GetN_FloatingCrystal) "None"))
  (for (_array_element _array_index) _returnvalue
    (if (== _array_index 0)
      (Variables|Default|SetPartical%20location _array_element))))

(fn SetRandomLoc
  (params (Target :type Scene%20Component%20Object%20Reference))
  (Transformation|SetRelativeLocation Target (Math|Vector|MakeVector (.x (Variables|/Script/Engine.SceneComponent|GetRelativeLocation Target)) (Math|Random|RandomFloatinRange -3e+01 2e+02) (Math|Random|RandomFloatinRange -3e+01 2e+02)) false true))