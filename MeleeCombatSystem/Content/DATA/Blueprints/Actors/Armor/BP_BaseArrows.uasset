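; Base equippable arrows item that shows the wearer's arrows as static meshes attached to its item mesh.
; On equip or update, if the item mesh is visible, it reads the player's first arrow inventory slot; other characters get a fixed large count.
; It then rebuilds collision-free meshes at predefined display locations, up to the arrow count.
; The rebuild is skipped while the display is full and arrows exceed its capacity.
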(event Custom|UpdateArrowCount
  (if (Rendering|IsVisible (Variables|Default|GetItemStaticMesh))
    (CallFunction|GetArrowCount)
    (CallFunction|VisualArrows)))

(event EventBeginPlay
  (|CallParentFunction) ; This node is disabled and will not be called.\nDrag off pins to build functionality.
)

(event Collision|EventActorBeginOverlap
  (params (OtherActor :type Actor%20Object%20Reference))
  (|CallParentFunction OtherActor) ; This node is disabled and will not be called.\nDrag off pins to build functionality.
)

(event EventTick
  (params (DeltaSeconds :type Float%20%28single-precision%29))
  (|CallParentFunction DeltaSeconds) ; This node is disabled and will not be called.\nDrag off pins to build functionality.
)

(event EventGenericAction
  (if (Rendering|IsVisible (Variables|Default|GetItemStaticMesh))
    (CallFunction|GetArrowCount)
    (CallFunction|VisualArrows)))

(fn ConstructionScript
  (|CallParentFunction))

(fn OnEquipped
  (|CallParentFunction)
  (CallFunction|UpdateArrowCount))

(fn VisualArrows
  (bind _displayeditems (Variables|Default|GetDisplayedItems))
  (if (not (>= (Utilities|Array|Length (Variables|Default|GetDisplayedItems)) (Utilities|Array|Length (Variables|Default|GetArrowDisplayLoc))))
    (bind _arrayelement (Utilities|Array|ReverseforEachLoop _displayeditems :!label _label)
      (:LoopBody
        (Components|DestroyComponent _arrayelement))
      (:Completed
        (Utilities|Array|Clear _displayeditems)
        (for _array_element (Variables|Default|GetArrowDisplayLoc)
          (if (> (Variables|Default|GetNumberOfArrows) (LocalVariables|GetSpawnCount))
            (Math|Integer|IncrementInt (LocalVariables|GetSpawnCount)
              (:%20%20
                (bind _returnvalue (AddComponent|AddStaticMeshComponent false (Math|Transform|MakeTransform (+ (.Location (Math|Transform|BreakTransform _array_element)) "0.000000,0.000000,-15.000000") (.Rotation (Math|Transform|BreakTransform _array_element)) "0.900000,1.000000,1.000000")))
                (Components|StaticMesh|SetStaticMesh _returnvalue (Variables|Default|GetCustomDropMesh))
                (Transformation|AttachComponentToComponent _returnvalue (Variables|Default|GetItemStaticMesh) "None" "KeepRelative" "KeepRelative" "KeepWorld" true)
                (Collision|SetCollisionEnabled _returnvalue "NoCollision")
                (Utilities|Array|Add (Variables|Default|GetDisplayedItems) _returnvalue)))))))
    (elif (<= (Variables|Default|GetNumberOfArrows) (Utilities|Array|Length (Variables|Default|GetArrowDisplayLoc)))
      (goto _label))))

(fn GetArrowCount
  (bind _equipped_character (Variables|Default|GetEquipped%20Character))
  (bind _inventory (Variables|/Game/DATA/BP_PC.BP_PC_C|GetInventory _equipped_character))
  (if (Variables|/Game/DATA/Blueprints/Components/CombatComponent.CombatComponent_C|GetIsPlayer (Variables|/Game/DATA/BP_PC.BP_PC_C|GetCombatComponent (Variables|Default|GetEquipped%20Character)))
    (Variables|Default|SetNumberOfArrows (.Amount (Default|GetSlotInfo _inventory (Variables|/Game/DATA/Blueprints/Actors/Inventory/BP_Inventory.BP_Inventory_C|GetArrowSlots _inventory))))
    (else
      (Variables|Default|SetNumberOfArrows 1000))))