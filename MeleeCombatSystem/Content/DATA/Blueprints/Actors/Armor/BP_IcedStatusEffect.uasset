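; BP_IcedStatusEffect is an equippable status effect that puts an iced state, named as a speed-down, on the character wearing it.
; On equip it calls the combat component's Iced, plays an ice sound, and attaches a Niagara body effect bound to the character's skeletal mesh plus a quiet looping-style wind sound.
; On unequip it calls the same Iced function again, deactivates the particles and fades out the wind.
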(event Custom|ApplySpeedDown
  (bind _equipped_character (Variables|Default|GetEquipped%20Character))
  (bind _equipped_character_2 (Variables|Default|GetEquipped%20Character))
  (bind _mesh (Variables|/Script/Engine.Character|GetMesh _equipped_character_2))
  (bind _mesh_2 (Variables|/Script/Engine.Character|GetMesh _equipped_character))
  (bind _returnvalue (Transformation|GetWorldLocation _mesh))
  (Default|Iced (Variables|/Game/DATA/BP_PC.BP_PC_C|GetCombatComponent (Variables|Default|GetEquipped%20Character)))
  (bind _returnvalue_2 (Niagara|SpawnSystemAttached "/Game/DATA/Effects/N_IceBody.N_IceBody" _mesh_2 "None" (Transformation|GetWorldLocation _mesh_2) "0, 0, 0" "KeepRelativeOffset" true))
  (bind _output_get (Variables|Default|SetEffect _returnvalue_2))
  (Class|NiagaraFunctionLibrary|OverrideSystemUserVariableSkeletalMeshComponent _output_get "SkeletalMesh" (Variables|/Script/Engine.Character|GetMesh (Variables|Default|GetEquipped%20Character)))
  (Audio|PlaySoundatLocation "/Game/DATA/SoundFX/WaterMagic/SC_Ice_IS_T1.SC_Ice_IS_T1" _returnvalue "0, 0, 0" 1.0 1.0 0.0 0 0 0 0)
  (bind _returnvalue_3 (Audio|SpawnSoundAttached "/Game/DATA/SoundFX/WaterMagic/SC_SnowWind.SC_SnowWind" (Variables|/Script/Engine.Character|GetMesh (Variables|Default|GetEquipped%20Character)) "None" _returnvalue "0, 0, 0" "KeepRelativeOffset" false 0.2 1.0 0.0 0 0))
  (Variables|Default|SetSoundEffect _returnvalue_3))

(event Custom|RemoveEffect
  (Components|Activation|Deactivate (Variables|Default|GetEffect))
  (Audio|Components|Audio|FadeOut (Variables|Default|GetSoundEffect) 1.0 0.0 "Linear" :!class /Script/Engine.AudioComponent))

(event EventBeginPlay
  (|CallParentFunction) ; This node is disabled and will not be called.\nDrag off pins to build functionality.
)

(event Collision|EventActorBeginOverlap
  (params (OtherActor :type Actor%20Object%20Reference))
  (|CallParentFunction OtherActor) ; This node is disabled and will not be called.\nDrag off pins to build functionality.
)

(event EventTick
  (params (DeltaSeconds :type Float%20%28single-precision%29))
  (|CallParentFunction DeltaSeconds) ; This node is disabled and will not be called.\nDrag off pins to build functionality.
)

(fn ConstructionScript
  (|CallParentFunction))

(fn OnEquipped
  (|CallParentFunction)
  (CallFunction|ApplySpeedDown))

(fn OnUnequipped
  (params (GiveBack? :type Boolean) (ForceDrop :type Boolean) (ItemInfoIn :type S%20Item%20Info%20Structure))
  (Default|Iced (Variables|/Game/DATA/BP_PC.BP_PC_C|GetCombatComponent (Variables|Default|GetEquipped%20Character)))
  (CallFunction|RemoveEffect)
  (|CallParentFunction GiveBack? ForceDrop ItemInfoIn))