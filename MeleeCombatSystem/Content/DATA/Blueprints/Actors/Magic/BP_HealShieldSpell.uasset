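; BP_HealShieldSpell is a spell actor that heals its caster and knocks other players away with an expanding shield.
; Shortly after spawn, it plays effects and sphere-traces for the caster, running the inherited ApplyDamage on it.
; In parallel, a timeline scales up the shield, then triggers the caster's jump input.
; Overlapping BP_PC characters other than the caster are launched upward, then outward after a delay.
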(event Custom|Heal
  (bind _returnvalue (Transformation|GetActorLocation))
  (Utilities|FlowControl|Sequence
    (:then_0
      (Transformation|SetWorldTransform (Variables|Default|GetP_Health_Player_Buff_Ping_01) (Transformation|GetActorTransform (Variables|Default|GetCharacter)) false true)
      (Components|Activation|Activate (Variables|Default|GetExplosiveSound) true)
      (bind _outhits (Collision|MultiSphereTraceForObjects _returnvalue _returnvalue 1e+02 (Utilities|Array|MakeArray "ObjectTypeQuery3") false 0 "None"))
      (bind _array_element (Utilities|Array|ForEachLoopwithBreak _outhits)
        (:LoopBody
          (if (== (.HitActor (Collision|BreakHitResult _array_element)) (Variables|Default|GetCharacter))
            (CallFunction|ApplyDamage (Variables|Default|GetCharacter) _array_element false 1.0)
            (CallFunction|Break)))
        (:Completed
          (Utilities|FlowControl|Delay 5.0)
          (Actor|DestroyActor))))
    (:then_1
      (Transformation|SetWorldLocation (Variables|Default|GetExpandingShield) (Transformation|GetWorldLocation (Variables|/Script/Engine.Character|GetMesh (Variables|Default|GetCharacter))) false true)
      (Components|Activation|Activate (Variables|Default|GetImpactSound) true)
      (bind _grow (Timeline|Grow PlayFromStart)
        (:Update
          (Transformation|SetWorldScale3D (Variables|Default|GetExpandingShield) (Math|Conversions|ToVector(Float) (Math|Float|Lerp 1e+01 5e+01 _grow))))
        (:Finished
          (Utilities|FlowControl|Delay 1.0)
          (Default|JumpInputPushed (Variables|/Game/DATA/BP_PC.BP_PC_C|GetCombatComponent (Variables|Default|GetCharacter)))
          (Utilities|FlowControl|Delay 1.0)
          (Components|DestroyComponent (Variables|Default|GetExpandingShield)))))
    (:then_2
      (for _array_element_2 (Collision|GetOverlappingActors (Variables|Default|GetAreaOfEffect) "/Game/DATA/BP_PC.BP_PC_C" :!class /Script/Engine.PrimitiveComponent)
        (if (!= (Variables|Default|GetCharacter) _array_element_2)
          (bind _asbp_pc (Utilities|Casting|CastToBP_PC _array_element_2))
          (Character|LaunchCharacter _asbp_pc "0.000000,0.000000,400.000000" true true)
          (Utilities|FlowControl|Delay 0.3)
          (Character|LaunchCharacter _asbp_pc (* (Math|Vector|GetForwardVector (Math|Rotator|FindLookatRotation (Transformation|GetActorLocation) (Transformation|GetActorLocation _asbp_pc))) 8.5e+02) true true))))))

(event Custom|Break
  (Utilities|Array|ForEachLoopwithBreak (stale Custom|Heal _outhits)) ; enters at Break
)

(event EventBeginPlay
  (|CallParentFunction)
  (Utilities|FlowControl|Delay 0.2)
  (CallFunction|Heal)
  (Collision|IgnoreActorwhenMoving (Variables|Default|GetExpandingShield) (Variables|Default|GetCharacter) true))

(event Collision|EventActorBeginOverlap
  (params (OtherActor :type Actor%20Object%20Reference)))

(event EventTick
  (params (DeltaSeconds :type Float%20%28single-precision%29))
  (|CallParentFunction DeltaSeconds) ; This node is disabled and will not be called.\nDrag off pins to build functionality.
)

(fn ConstructionScript
  (|CallParentFunction))