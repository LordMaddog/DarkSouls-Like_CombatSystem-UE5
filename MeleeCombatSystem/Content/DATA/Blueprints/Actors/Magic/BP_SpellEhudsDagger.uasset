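; Ehud's Dagger spell projectile, which homes in on the target's mesh and damages what it hits.
; On a character it sticks to the hit bone and spawns BP_PoopSpell at a downward trace behind the target; otherwise it plays a blast effect.
; It notifies its Spawner via ArtifactSpellDoneMessage before self-destructing on hit or lifetime timeout.
; Explosion, shrink, ice decal and size-scaling logic is disconnected and never runs.
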(event Custom|ExplodOnImpact!
  ;[1 1 1] Explode when damaged.
)

(event EventBeginPlay
  (Variables|/Script/Engine.ProjectileMovementComponent|SetHomingTargetComponent (Variables|Default|GetProjectileMovement) (Variables|/Script/Engine.Character|GetMesh (Variables|Default|GetTarget)))
  (|CallParentFunction)
  (Variables|/Script/Engine.ProjectileMovementComponent|SetHomingAccelerationMagnitude (Variables|Default|GetProjectileMovement) 3e+02)
  (Utilities|FlowControl|Delay 8.0)
  (Class|CombatBPI|ArtifactSpellDone(Message) (Variables|Default|GetSpawner))
  (Actor|DestroyActor))

(event Collision|EventActorBeginOverlap
  (params (OtherActor :type Actor%20Object%20Reference)))

(event Game|Damage|EventAnyDamage
  (params (Damage :type Float%20%28single-precision%29) (DamageType :type Damage%20Type%20Object%20Reference) (InstigatedBy :type Controller%20Object%20Reference) (DamageCauser :type Actor%20Object%20Reference))
  ;[1 1 1] Explode when damaged.
)

(event EventTick
  (params (DeltaSeconds :type Float%20%28single-precision%29))
  ;[1 1 1] Strink
)

(event EventHit
  (bind _character (Variables|Default|GetCharacter))
  (bind _target (Variables|Default|GetTarget))
  (bind _returnvalue (Transformation|GetActorForwardVector _target))
  (bind _returnvalue_2 (Transformation|GetActorLocation _target))
  (bind _returnvalue_3 (* _returnvalue -2e+02))
  (bind _returnvalue_4 (+ _returnvalue_2 _returnvalue_3))
  ;[1 1 1] Hit
  (|CallParentFunction)
  (Utilities|FlowControl|DoOnce false
    (:Completed
      (Niagara|SetNiagaraVariable(Float) (Variables|Default|GetN_Ice_Trail) "Spawn Spacing" 0.0)
      (Components|Activation|Activate (Variables|Default|GetImpactSound) true)
      (Audio|Components|Audio|Stop (Variables|Default|GetFlySound))
      (CallFunction|ApplyDamage (Variables|Default|GetHitActor) (Variables|Default|GetHitInfo) false 1.0)
      (bind _ascharacter (Utilities|Casting|CastToCharacter (Variables|Default|GetHitActor))
        (:then
          (Transformation|AttachComponentToComponent (Variables|Default|GetMainProjectileCore) (Variables|/Script/Engine.Character|GetMesh _ascharacter) (.HitBoneName (Collision|BreakHitResult (Variables|Default|GetHitInfo))) "KeepWorld" "KeepWorld" "KeepWorld" true)
          (Collision|SetCollisionResponsetoChannel (Variables|Default|GetVisualEffect) "ECC_Pawn" "ECR_Ignore")
          (Collision|SetCollisionResponsetoChannel (Variables|Default|GetVisualEffect) "ECC_Visibility" "ECR_Ignore")
          (Collision|SetCollisionResponsetoChannel (Variables|Default|GetVisualEffect) "ECC_Camera" "ECR_Ignore")
          (Collision|SetCollisionResponsetoChannel (Variables|Default|GetVisualEffect) "ECC_GameTraceChannel2" "ECR_Block")
          (bind _outhit (Collision|LineTraceByChannel _returnvalue_4 (+ _returnvalue_4 "0.000000,0.000000,-450.000000") "TraceTypeQuery1" false (Utilities|Array|MakeArray (Variables|Default|GetTarget)) "None"))
          (Game|SpawnActorfromClass "/Game/DATA/Blueprints/Actors/Magic/BP_PoopSpell.BP_PoopSpell_C" (Math|Transform|MakeTransform (.location _outhit) "0, 0, 0" "1.000000,1.000000,1.000000") "Undefined" "MultiplyWithRoot" _character _character _character)
          (Utilities|FlowControl|Delay 7.0)
          (Class|CombatBPI|ArtifactSpellDone(Message) (Variables|Default|GetSpawner))
          (Actor|DestroyActor))
        (:CastFailed
          (Components|Activation|Activate (Variables|Default|GetTeleportParticelsBlast_System) false)
          (Class|CombatBPI|ArtifactSpellDone(Message) (Variables|Default|GetSpawner) 1)
          (Utilities|FlowControl|Delay 1.0)
          (Actor|DestroyActor))))))

(fn ConstructionScript
  ;[1 1 1] Set size and area of effect
  (|CallParentFunction))