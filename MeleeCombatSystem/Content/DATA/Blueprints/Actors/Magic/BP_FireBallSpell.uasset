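; Fireball spell actor whose size, effects, volume and force radius scale with damage and area of effect, with damage derived from a caster sub-stat.
; Hit, also fired 30 seconds after spawn, staggers overlapping BP_PC actors and chains timelines.
; The ball implodes, pulling those actors to the hit location, then expands into an explosion that damages all overlapping actors.
; A sphere trace then spawns scorch decals before the ball shrinks and destroys itself.
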(event Custom|Grow
  (bind _mainprojectilecore (Variables|Default|GetMainProjectileCore))
  (bind _damageout (Variables|Default|GetDamageOut))
  (bind _areaeffect (Variables|Default|GetAreaEffect))
  (bind _mainprojectilecore_2 (Variables|Default|GetMainProjectileCore))
  (bind _returnvalue (* _areaeffect 0.5))
  (bind _returnvalue_2 (* _damageout _returnvalue))
  (bind _returnvalue_3 (* _returnvalue_2 1.2))
  ;[1 1 1] Grow
  (Transformation|SetWorldScale3D (Variables|Default|GetMainProjectileCore) (Math|Conversions|ToVector(Float) _returnvalue_2))
  (Niagara|SetNiagaraVariable(Float) (Variables|Default|GetN_FireBall) "Scale" (* _returnvalue_2 0.1))
  (Niagara|SetNiagaraVariable(Float) (Variables|Default|GetN_FireBall) "FScale" (* _returnvalue_2 2.0))
  (Niagara|SetNiagaraVariable(Float) (Variables|Default|GetN_FireBall) "Spawn Rate" (* _returnvalue_2 0.3))
  (Components|Sphere|SetSphereRadius (Variables|Default|GetAreaOfEffect) (Math|Float|Clamp(Float) _returnvalue_3 2e+01 _returnvalue_3) false)
  (Variables|/Script/Engine.AudioComponent|SetVolumeMultiplier (Variables|Default|GetSC_Explosion) _returnvalue_2)
  (Variables|/Script/Engine.AudioComponent|SetVolumeMultiplier (Variables|Default|GetSC_Fire) _returnvalue_2)
  (Variables|/Script/Engine.AudioComponent|SetVolumeMultiplier (Variables|Default|GetSC_AirSuck) _returnvalue_2)
  (Variables|/Script/Engine.RadialForceComponent|SetRadius (Variables|Default|GetRadialForce) (* _returnvalue_2 5e+01))
  (if (> (Variables|Default|GetDamageOut) 2e+01)
    (Transformation|SetRelativeLocation _mainprojectilecore (+ (Variables|/Script/Engine.SceneComponent|GetRelativeLocation _mainprojectilecore) "1.000000,0.000000,0.000000") false false)
    (if (> (Variables|Default|GetDamageOut) 5e+01)
      (Transformation|SetRelativeLocation _mainprojectilecore_2 (+ (Variables|/Script/Engine.SceneComponent|GetRelativeLocation _mainprojectilecore_2) "1.000000,0.000000,0.000000") false false))))

(event EventBeginPlay
  (|CallParentFunction)
  (Utilities|FlowControl|Delay 3e+01)
  (CallFunction|Hit))

(event Collision|EventActorBeginOverlap
  (params (OtherActor :type Actor%20Object%20Reference)))

(event EventTick
  (params (DeltaSeconds :type Float%20%28single-precision%29))
  (|CallParentFunction DeltaSeconds))

(event EventHit
  ;[1 1 1] Hit
  (for _array_element (Collision|GetOverlappingActors (Variables|Default|GetAreaOfEffect) "/Game/DATA/BP_PC.BP_PC_C" :!class /Script/Engine.PrimitiveComponent)
    (Default|PerformHitReaction (Actor|GetComponentbyClass _array_element "/Game/DATA/Blueprints/Components/CombatComponent.CombatComponent_C") false true "NewEnumerator0"))
  (Variables|Default|SetexplosionSize (* (Variables|Default|GetDamageOut) 0.5))
  (Class|RadialForceComponent|FireImpulse (Variables|Default|GetRadialForce))
  (Components|Activation|Activate (Variables|Default|GetN_FieryVacuum) false)
  (bind _shrink (Timeline|Shrink PlayFromStart)
    (:Update
      (Niagara|SetNiagaraVariable(Float) (Variables|Default|GetN_FireBall) "Scale" (Math|Float|Lerp (* (Variables|Default|GetexplosionSize) 0.1) 0.0 _shrink))
      (Transformation|SetWorldScale3D (Variables|Default|GetMainProjectileCore) (Math|Conversions|ToVector(Float) (Math|Float|Lerp (Variables|Default|GetexplosionSize) 0.0 _shrink)))
      (Components|Activation|Activate (Variables|Default|GetSC_AirSuck) false)
      (for _array_element_2 (Collision|GetOverlappingActors (Variables|Default|GetAreaOfEffect) "/Game/DATA/BP_PC.BP_PC_C" :!class /Script/Engine.PrimitiveComponent)
        (Transformation|SetActorLocation _array_element_2 (Math|Vector|Lerp(Vector) (Transformation|GetActorLocation _array_element_2) (.Location (Collision|BreakHitResult (Variables|Default|GetHitInfo))) _shrink) true false)))
    (:Finished
      (Variables|/Script/Engine.RadialForceComponent|SetImpulseStrength (Variables|Default|GetRadialForce) 2.4e+04)
      (bind _shrink_2 (Timeline|GrowBoom PlayFromStart)
        (:Update
          (Niagara|SetNiagaraVariable(Float) (Variables|Default|GetN_FireBall) "Scale" (Math|Float|Lerp 0.0 (* (Variables|Default|GetexplosionSize) 0.3) _shrink_2))
          (Transformation|SetWorldScale3D (Variables|Default|GetMainProjectileCore) (Math|Conversions|ToVector(Float) (Math|Float|Lerp 0.0 (* (Variables|Default|GetexplosionSize) 1.4) _shrink_2)))
          (Components|Activation|Activate (Variables|Default|GetSC_Explosion) false))
        (:Finished
          (for _array_element_3 (Collision|GetOverlappingActors (Variables|Default|GetAreaOfEffect) 0 :!class /Script/Engine.PrimitiveComponent)
            (CallFunction|ApplyDamage _array_element_3 (Variables|Default|GetHitInfo) true)
            (Class|RadialForceComponent|FireImpulse (Variables|Default|GetRadialForce)))
          ;[1 1 1] End-Self delete and spawn decal
          (CallFunction|Decal)
          (bind _shrink_3 (Timeline|Timeline PlayFromStart)
            (:Update
              (Niagara|SetNiagaraVariable(Float) (Variables|Default|GetN_FireBall) "Scale" (Math|Float|Lerp (* (Variables|Default|GetexplosionSize) 0.1) 0.0 _shrink_3))
              (Transformation|SetWorldScale3D (Variables|Default|GetMainProjectileCore) (Math|Conversions|ToVector(Float) (Math|Float|Lerp (Variables|Default|GetexplosionSize) 0.0 _shrink_3))))
            (:Finished
              (Utilities|FlowControl|Delay 0.5)
              (Actor|DestroyActor))))))))

(fn ConstructionScript
  (|CallParentFunction))

(fn AddDamage
  (params (DamageMultiplier :type Float%20%28double-precision%29))
  (bind _output_get (Variables|Default|SetDamageOut (* DamageMultiplier (Default|GetSubStats (Variables|/Game/DATA/BP_PC.BP_PC_C|GetStatsComponent (Variables|Default|GetCharacter)) "NewEnumerator12"))))
  (return _output_get))

(fn Decal
  (bind _mainprojectilecore (Variables|Default|GetMainProjectileCore))
  (bind _returnvalue (Transformation|GetWorldLocation _mainprojectilecore))
  (bind _outhits (Collision|MultiSphereTraceByChannel _returnvalue _returnvalue (* (Variables|Default|GetDamageOut) (* (Variables|Default|GetAreaEffect) 4.0)) "TraceTypeQuery1" false (Utilities|Array|MakeArray 0) "None" true "(R=1.000000,G=0.000000,B=0.000000,A=1.000000)" "(R=0.000000,G=1.000000,B=0.000000,A=1.000000)" 15.0))
  (for _array_element _outhits
    (if (.bBlockingHit (Collision|BreakHitResult _array_element))
      (Utilities|IsValid (Actor|GetComponentbyClass (.HitActor (Collision|BreakHitResult _array_element)) "/Game/DATA/Blueprints/Components/CombatComponent.CombatComponent_C")
        (:Is%20Valid
          (bind _returnvalue_2 (Default|CanReciveDamage (Actor|GetComponentbyClass (.HitActor (Collision|BreakHitResult _array_element)) "/Game/DATA/Blueprints/Components/CombatComponent.CombatComponent_C")))
          (if _returnvalue_2
            (CallFunction|SpawnDecal _array_element "/Game/DATA/Blueprints/Decals/BP_FireBallDecal.BP_FireBallDecal_C" 1.0 true (Math|Conversions|ToVector(Float) (* (Variables|Default|GetexplosionSize) 0.05)))))
        (:Is%20Not%20Valid
          (Utilities|IsValid (Actor|GetComponentbyClass (.HitActor (Collision|BreakHitResult _array_element)) "/Game/DATA/Blueprints/Components/inanimateObjectStats.inanimateObjectStats_C")
            (:Is%20Valid
              (bind _returnvalue_3 (Default|CanReciveDamage (Actor|GetComponentbyClass (.HitActor (Collision|BreakHitResult _array_element)) "/Game/DATA/Blueprints/Components/inanimateObjectStats.inanimateObjectStats_C")))
              (if _returnvalue_3
                (CallFunction|SpawnDecal _array_element "/Game/DATA/Blueprints/Decals/BP_FireBallDecal.BP_FireBallDecal_C" 1.0 true (Math|Conversions|ToVector(Float) (* (Variables|Default|GetexplosionSize) 0.05)))))
            (:Is%20Not%20Valid
              (CallFunction|SpawnDecal _array_element "/Game/DATA/Blueprints/Decals/BP_FireBallDecal.BP_FireBallDecal_C" 1.0 true (Math|Conversions|ToVector(Float) (* (Variables|Default|GetexplosionSize) 0.15))))))))))