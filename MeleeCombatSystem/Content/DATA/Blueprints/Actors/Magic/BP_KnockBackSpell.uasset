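; Knockback spell actor that plays a wave effect and explosive sound, then launches overlapping player characters other than its own Character.
; On BeginPlay it scales the Niagara wave and radial force radius from AreaEffect, then triggers Boom after a short delay.
; Boom uses LaunchCharacter to pop targets upward, then, after a Delay inside the loop, away from the spell, and later destroys itself.
; The RadialForce impulse is disconnected.
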(event Custom|Boom
  (Components|Activation|Activate (Variables|Default|GetN_KnockBackwave) true)
  (for _array_element (Collision|GetOverlappingActors (Variables|Default|GetAreaOfEffect) "/Game/DATA/BP_PC.BP_PC_C" :!class /Script/Engine.PrimitiveComponent)
    (if (!= (Variables|Default|GetCharacter) _array_element)
      (bind _asbp_pc (Utilities|Casting|CastToBP_PC _array_element))
      (Character|LaunchCharacter _asbp_pc "0.000000,0.000000,400.000000" true true)
      (Utilities|FlowControl|Delay 0.3)
      (Character|LaunchCharacter _asbp_pc (* (Math|Vector|GetForwardVector (Math|Rotator|FindLookatRotation (Transformation|GetActorLocation) (Transformation|GetActorLocation _asbp_pc))) 7e+02) true true)))
  (Utilities|FlowControl|Delay 5.0)
  (Actor|DestroyActor))

(event EventBeginPlay
  (|CallParentFunction)
  (Variables|/Script/Engine.RadialForceComponent|SetRadius (Variables|Default|GetRadialForce) (* (Variables|Default|GetAreaEffect) 2.0))
  (Niagara|SetNiagaraVariable(Float) (Variables|Default|GetN_KnockBackwave) "Size" (* (Variables|Default|GetAreaEffect) 3.0))
  (Utilities|FlowControl|Delay 0.2)
  (CallFunction|Boom))

(event Collision|EventActorBeginOverlap
  (params (OtherActor :type Actor%20Object%20Reference)))

(event EventTick
  (params (DeltaSeconds :type Float%20%28single-precision%29))
  (|CallParentFunction DeltaSeconds) ; This node is disabled and will not be called.\nDrag off pins to build functionality.
)

(fn ConstructionScript)