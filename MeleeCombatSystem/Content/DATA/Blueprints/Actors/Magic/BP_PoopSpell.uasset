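; BP_PoopSpell is a magic spell actor that acts as a slippery poop hazard, playing a plop on spawn and destroying itself after fifteen seconds.
; Its sphere overlap affects any BP_PC other than the stored Character, breaking its poise and activating a slip sound.
; If the victim is flying, it first calls Fly on their CombatComponent, apparently to toggle flight off, and briefly waits before the poise break.
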(event OnComponentBeginOverlap(Sphere)
  (params (OverlappedComponent :type Primitive%20Component%20Object%20Reference) (OtherActor :type Actor%20Object%20Reference) (OtherComp :type Primitive%20Component%20Object%20Reference) (OtherBodyIndex :type Integer) (bFromSweep :type Boolean) (SweepResult :type Hit%20Result%20Structure%20%28by%20ref%29))
  (bind _asbp_pc (Utilities|Casting|CastToBP_PC OtherActor))
  (if (!= _asbp_pc (Variables|Default|GetCharacter))
    (if (not (Variables|/Game/DATA/Blueprints/Components/CombatComponent.CombatComponent_C|GetbFlying (Variables|/Game/DATA/BP_PC.BP_PC_C|GetCombatComponent _asbp_pc)))
      _
      (else
        (Default|Fly (Variables|/Game/DATA/BP_PC.BP_PC_C|GetCombatComponent _asbp_pc))
        (Utilities|FlowControl|Delay 0.2)))
    (Default|PoiseBreak _asbp_pc)
    (Components|Activation|Activate (Variables|Default|GetSC_slip_in_poop) false)))

(event EventBeginPlay
  (Components|Activation|Activate (Variables|Default|GetSC_PoopPlop) false)
  (Utilities|FlowControl|Delay 15.0)
  (Actor|DestroyActor))

(event Collision|EventActorBeginOverlap
  (params (OtherActor :type Actor%20Object%20Reference)))

(event EventTick
  (params (DeltaSeconds :type Float%20%28single-precision%29)))

(fn ConstructionScript)