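; BP_PowerSlice is a magic area attack that knocks back and damages the actors it overlaps.
; Shortly after BeginPlay it checks AreaOfEffect once, pushing Characters away from the Instigator with a velocity-change impulse plus lift.
; Each overlapped actor takes damage using hit info from a sphere trace cast from the Instigator.
; A delayed destroy sits inside the overlap loop, so it only runs when something was overlapped.
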(event EventBeginPlay
  (|CallParentFunction)
  (Utilities|FlowControl|Delay 0.2)
  (for _array_element (Collision|GetOverlappingActors (Variables|Default|GetAreaOfEffect) 0 :!class /Script/Engine.PrimitiveComponent)
    (CallFunction|KnockBack _array_element)
    (bind _outhit (CallFunction|GetHitInfo _array_element))
    (CallFunction|ApplyDamage _array_element _outhit true 1.0)
    (Utilities|FlowControl|Delay 4.0)
    (Actor|DestroyActor)))

(event Collision|EventActorBeginOverlap
  (params (OtherActor :type Actor%20Object%20Reference)))

(event EventTick
  (params (DeltaSeconds :type Float%20%28single-precision%29))
  (|CallParentFunction DeltaSeconds) ; This node is disabled and will not be called.\nDrag off pins to build functionality.
)

(fn ConstructionScript
  (|CallParentFunction))

(fn KnockBack
  (params (Target :type Actor%20Object%20Reference))
  (bind _ascharacter (Utilities|Casting|CastToCharacter Target))
  (Physics|AddImpulse (Variables|/Script/Engine.Character|GetCharacterMovement _ascharacter) (+ (* (Math|Rotator|FindLookatRotation (Transformation|GetActorLocation (Variables|Default|GetInstigator)) (Transformation|GetActorLocation _ascharacter)) 1.5e+03) "0.000000,0.000000,350.000000") true))

(fn GetHitInfo
  (params (Target :type Actor%20Object%20Reference))
  (bind _outhit (Collision|SphereTraceForObjects (Transformation|GetActorLocation (Variables|Default|GetInstigator)) (Transformation|GetActorLocation Target) 1e+01 (Utilities|Array|MakeArray "ObjectTypeQuery9" "ObjectTypeQuery8" "ObjectTypeQuery4") false (Utilities|Array|MakeArray (Variables|Default|GetInstigator)) (Variables|/Game/DATA/Blueprints/Components/CombatComponent.CombatComponent_C|GetDraw%20Debug%20Type (Variables|/Game/DATA/BP_PC.BP_PC_C|GetCombatComponent (Variables|Default|GetCharacter)))))
  (return _outhit))

(fn GetPoiseDamageMutltiplier
  (return (* (Variables|Default|GetBasePoiseDamgeMultiplier) (Variables|Default|GetPoiseDamgeMultiplier))))