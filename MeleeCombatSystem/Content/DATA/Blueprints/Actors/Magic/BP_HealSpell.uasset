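; Heal spell actor that targets its Character, built on a parent class.
; Shortly after BeginPlay it moves a buff particle to the Character and activates it with a sound.
; A sphere trace for pawns at the actor's location filters hits to that Character and passes them to ApplyDamage without skill XP; HealPower is unused here.
; The actor destroys itself after a delay.
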(event Custom|Heal
  (bind _returnvalue (Transformation|GetActorLocation))
  (Transformation|SetWorldTransform (Variables|Default|GetP_Health_Player_Buff_Ping_01) (Transformation|GetActorTransform (Variables|Default|GetCharacter)) false true)
  (Components|Activation|Activate (Variables|Default|GetExplosiveSound) true)
  (bind _outhits (Collision|MultiSphereTraceForObjects _returnvalue _returnvalue 1e+02 (Utilities|Array|MakeArray "ObjectTypeQuery3") false 0 "None"))
  (bind _array_element (Utilities|Array|ForEachLoopwithBreak _outhits)
    (:LoopBody
      (if (== (.HitActor (Collision|BreakHitResult _array_element)) (Variables|Default|GetCharacter))
        (CallFunction|ApplyDamage (.HitActor (Collision|BreakHitResult _array_element)) _array_element false 1.0)))
    (:Completed
      (Utilities|FlowControl|Delay 5.0)
      (Actor|DestroyActor))))

(event Custom|Break
  (Utilities|Array|ForEachLoopwithBreak (stale Custom|Heal _outhits)) ; enters at Break
)

(event EventBeginPlay
  (|CallParentFunction)
  (Utilities|FlowControl|Delay 0.2)
  (CallFunction|Heal))

(event Collision|EventActorBeginOverlap
  (params (OtherActor :type Actor%20Object%20Reference)))

(event EventTick
  (params (DeltaSeconds :type Float%20%28single-precision%29))
  (|CallParentFunction DeltaSeconds) ; This node is disabled and will not be called.\nDrag off pins to build functionality.
)

(fn ConstructionScript
  (|CallParentFunction))