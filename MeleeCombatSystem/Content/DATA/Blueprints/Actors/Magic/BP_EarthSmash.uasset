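; BP_EarthSmash is an earth magic projectile that deals area damage on impact.
; The first hit on its core activates the Niagara-style smash effect, particle systems and explosion sound.
; It then applies damage, flagged to grant skill XP, to every actor overlapping its area-of-effect volume.
; The actor destroys itself after a short delay.
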(event OnComponentHit(MainProjectileCore)
  (params (HitComponent :type Primitive%20Component%20Object%20Reference) (OtherActor :type Actor%20Object%20Reference) (OtherComp :type Primitive%20Component%20Object%20Reference) (NormalImpulse :type Vector :default "0, 0, 0") (Hit :type Hit%20Result%20Structure%20%28by%20ref%29))
  (Variables|Default|SetHitInfo Hit)
  (Variables|Default|SetHitActor 0)
  (Utilities|FlowControl|DoOnce false
    (:Completed
      (Components|Activation|Activate (Variables|Default|GetN_EarthSmash) false)
      (for _array_element (Collision|GetOverlappingActors (Variables|Default|GetAreaOfEffect) 0 :!class /Script/Engine.PrimitiveComponent)
        (CallFunction|ApplyDamage _array_element (Variables|Default|GetHitInfo) true))
      (Utilities|FlowControl|Delay 4.0)
      (Actor|DestroyActor))))

(event EventBeginPlay
  (|CallParentFunction))

(event Collision|EventActorBeginOverlap
  (params (OtherActor :type Actor%20Object%20Reference)))

(event EventTick
  (params (DeltaSeconds :type Float%20%28single-precision%29))
  (|CallParentFunction DeltaSeconds) ; This node is disabled and will not be called.\nDrag off pins to build functionality.
)

(fn ConstructionScript
  (|CallParentFunction))