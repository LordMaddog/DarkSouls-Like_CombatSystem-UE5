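; Lightning beam spell that fires from the caster's hand socket, damaging targets at the impact point and chaining onward.
; Tick runs a two-stage sphere trace, aim view then hand, to set the Niagara beam end and trigger throttled hits.
; Hits sphere-trace an AreaEffect-scaled radius for decals and damage, then search wider to spawn one weaker BP_lightningChainSpell at a time on another damageable target.
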(event Custom|OnHit
  (params (LOC :type Vector))
  ;[1 1 1] Damage And Decal
  (bind _outhits (Collision|MultiSphereTraceForObjects LOC LOC (* (Variables|Default|GetAreaEffect) 6.0) (Utilities|Array|MakeArray "ObjectTypeQuery1" "ObjectTypeQuery4" "ObjectTypeQuery9" "ObjectTypeQuery6" "ObjectTypeQuery8" "ObjectTypeQuery5") false (Utilities|Array|MakeArray (Variables|Default|GetCharacter) self) "None"))
  (for _array_element _outhits
    (if (.bBlockingHit (Collision|BreakHitResult _array_element))
      (CallFunction|Decal _array_element)
      (Utilities|IsValid (Actor|GetComponentbyClass (.HitActor (Collision|BreakHitResult _array_element)) "/Game/DATA/Blueprints/Components/CombatComponent.CombatComponent_C")
        (:Is%20Valid
          (bind _returnvalue (Default|CanReciveDamage (Actor|GetComponentbyClass (.HitActor (Collision|BreakHitResult _array_element)) "/Game/DATA/Blueprints/Components/CombatComponent.CombatComponent_C")))
          (if _returnvalue
            (bind _output_get (Variables|Default|SetDamageTemp (+ (* (Variables|Default|GetDamageOut) 0.5) (Variables|Default|GetDamageTemp)) :!label _label))
            (if (>= _output_get (Variables|Default|GetDamageOut))
              (Variables|Default|SetDamageTemp 0.0)
              (Utilities|FlowControl|DoOnce false :!label _label_2
                (:Completed
                  (Utilities|FlowControl|Sequence
                    (:then_0
                      (CallFunction|ApplyDamage (.HitActor (Collision|BreakHitResult _array_element)) _array_element true 0.3)
                      (Variables|Default|SetHitTarget (.HitActor (Collision|BreakHitResult _array_element)))
                      (Variables|Default|SetHitSomething true)
                      (CallFunction|Chain LOC))
                    (:then_1
                      (Utilities|FlowControl|Delay 0.2)
                      (goto _label_2 Reset))))))))
        (:Is%20Not%20Valid
          (Utilities|IsValid (Actor|GetComponentbyClass (.HitActor (Collision|BreakHitResult _array_element)) "/Game/DATA/Blueprints/Components/inanimateObjectStats.inanimateObjectStats_C")
            (:Is%20Valid
              (bind _returnvalue_2 (Default|CanReciveDamage (Actor|GetComponentbyClass (.HitActor (Collision|BreakHitResult _array_element)) "/Game/DATA/Blueprints/Components/inanimateObjectStats.inanimateObjectStats_C")))
              (if _returnvalue_2
                (goto _label))))))))
  (if (not (Variables|Default|GetHitSomething))
    (Variables|Default|SetHitTarget 0)
    (CallFunction|Chain LOC)
    (else
      (Variables|Default|SetHitSomething false))))

(event Custom|Chain
  (params (LOC :type Vector))
  ;[1 1 1] Chain
  (if (not (Utilities|IsValid (Variables|Default|GetSpawnedChain)))
    (bind _outhits (Collision|MultiSphereTraceForObjects LOC LOC (* (Variables|Default|GetAreaEffect) 1e+02) (Utilities|Array|MakeArray "ObjectTypeQuery1" "ObjectTypeQuery4" "ObjectTypeQuery9" "ObjectTypeQuery6" "ObjectTypeQuery8" "ObjectTypeQuery5") false (Utilities|Array|MakeArray (Variables|Default|GetCharacter) self) "None"))
    (for _array_element _outhits
      (if (and (.bBlockingHit (Collision|BreakHitResult _array_element)) (not (Utilities|IsValid (Variables|Default|GetSpawnedChain))))
        (Utilities|IsValid (Actor|GetComponentbyClass (.HitActor (Collision|BreakHitResult _array_element)) "/Game/DATA/Blueprints/Components/CombatComponent.CombatComponent_C")
          (:Is%20Valid
            (bind _returnvalue (Default|CanReciveDamage (Actor|GetComponentbyClass (.HitActor (Collision|BreakHitResult _array_element)) "/Game/DATA/Blueprints/Components/CombatComponent.CombatComponent_C")))
            (if _returnvalue
              (if (not (== (Variables|Default|GetHitTarget) (.HitActor (Collision|BreakHitResult _array_element)))) :!label _label
                (Variables|Default|GetTarget
                  (:then
                    (if (< (Variables|Default|GetDisttanceToCHainTarget) (Transformation|GetDistanceTo (.HitActor (Collision|BreakHitResult _array_element)) (Variables|Default|GetTarget)))
                      (Variables|Default|SetDisttanceToCHainTarget (Transformation|GetDistanceTo (.HitActor (Collision|BreakHitResult _array_element)) (Variables|Default|GetTarget)) :!label _label_2)
                      (Variables|Default|SetTarget (.HitActor (Collision|BreakHitResult _array_element)))))
                  (:else
                    (goto _label_2))))))
          (:Is%20Not%20Valid
            (Utilities|IsValid (Actor|GetComponentbyClass (.HitActor (Collision|BreakHitResult _array_element)) "/Game/DATA/Blueprints/Components/inanimateObjectStats.inanimateObjectStats_C")
              (:Is%20Valid
                (bind _returnvalue_2 (Default|CanReciveDamage (Actor|GetComponentbyClass (.HitActor (Collision|BreakHitResult _array_element)) "/Game/DATA/Blueprints/Components/inanimateObjectStats.inanimateObjectStats_C")))
                (if _returnvalue_2
                  (goto _label))))))))
    (CallFunction|Spawn LOC)))

(event Custom|Spawn
  (params (StarLoc :type Vector))
  (bind _character (Variables|Default|GetCharacter))
  ;[1 1 1] SpawnChain
  (Variables|Default|GetTarget
    (:then
      (if (not (Utilities|IsValid (Variables|Default|GetSpawnedChain)))
        (bind _returnvalue (Game|SpawnActorfromClass "/Game/DATA/Blueprints/Actors/Magic/BP_lightningChainSpell.BP_lightningChainSpell_C" (Math|Transform|MakeTransform (Transformation|GetActorLocation (Variables|Default|GetTarget)) "0, 0, 0" "1.000000,1.000000,1.000000") "Undefined" "MultiplyWithRoot" _character (Variables|Default|GetTarget) StarLoc (Variables|Default|GetHitTarget) (* (Variables|Default|GetDamageMultiplier) 0.7) (* (Variables|Default|GetAreaEffect) 0.5) 9e+04 0.0 _character (Variables|Default|GetBasePoiseDamgeMultiplier) false "(TagName=\"Character.Action.Skill/Magic.Lightning\")" false 0.0 _character))
        (Variables|Default|SetSpawnedChain _returnvalue)
        (Variables|Default|SetTarget 0)))
    (:else)))

(event EventBeginPlay
  ;[1 1 1] Event Begin Play
  (|CallParentFunction)
  (Components|Activation|Activate (Variables|Default|GetTrail) false)
  (Variables|Default|SetIsPlayer (Variables|/Game/DATA/Blueprints/Components/CombatComponent.CombatComponent_C|GetIsPlayer (Variables|/Game/DATA/BP_PC.BP_PC_C|GetCombatComponent (Variables|Default|GetCharacter))))
  (Transformation|AttachComponentToComponent (Variables|Default|GetMainProjectileCore) (Variables|/Script/Engine.Character|GetMesh (Variables|Default|GetCharacter)) "RHFS" "SnapToTarget" "KeepRelative" "KeepRelative" true)
  (Effects|Components|ParticleSystem|SetFloatParameter (Variables|Default|GetTrail) "Scale" (Variables|Default|GetAreaEffect))
  (Audio|Components|Audio|SetVolumeMultiplier (Variables|Default|GetFlySound) (Variables|Default|GetAreaEffect) :!class /Script/Engine.AudioComponent))

(event EventTick
  (params (DeltaSeconds :type Float%20%28single-precision%29))
  ;[1 1 1] Event Tick (sets beam start and end point)
  (Variables|Default|GetTrail
    (:then
      (Transformation|SetWorldLocation (Variables|Default|GetMainProjectileCore) (Transformation|GetSocketLocation (Variables|/Script/Engine.Character|GetMesh (Variables|Default|GetCharacter)) "RHFS") false true)
      (bind (_returnvalue _hit) (CallFunction|GetAimTrace (Variables|/Game/DATA/BP_PC.BP_PC_C|GetFollowCamera (Variables|Default|GetCharacter)) (Variables|Default|GetMainProjectileCore) (Variables|Default|GetMaxRange) 1e+01 "None" true "RHFS" (Utilities|Array|MakeArray (Variables|Default|GetCharacter) self)))
      (if _hit
        (Utilities|FlowControl|Sequence
          (:then_0
            _)
          (:then_1
            (Utilities|FlowControl|DoOnce false :!label _label
              (:Completed
                (CallFunction|OnHit (.Location (Math|Transform|BreakTransform _returnvalue)))
                (Utilities|FlowControl|Delay 0.51)
                (goto _label Reset))))))
      (Niagara|SetNiagaraVariable(Vector3) (Variables|Default|GetTrail) "Beam End" (.Location (Math|Transform|BreakTransform _returnvalue))))
    (:else)))

(fn ConstructionScript
  (|CallParentFunction))

(fn ActivateonOFF
  (params (On :type Boolean) (Target :type Actor%20Component%20Object%20Reference))
  (if On
    (if (not (Components|Activation|IsActive Target))
      (Components|Activation|SetActive Target true false))
    (elif (Components|Activation|IsActive Target)
      (Components|Activation|SetActive Target false false))))

(fn GetAimTrace
  (params (CameraTrace :type Scene%20Component%20Object%20Reference) (CastLocTrace :type Scene%20Component%20Object%20Reference) (TraceRange :type Float%20%28single-precision%29) (Radius :type Float%20%28single-precision%29) (DrawDebugType :type EDrawDebugTrace%20Enum :default "None") (SocketType :type Boolean) (InSocketName :type Name) (ActorsToIgnore :type Array%20of%20Actor%20Object%20References))
  (bind _returnvalue (Transformation|GetWorldLocation CameraTrace))
  (bind _returnvalue_2 (Math|Vector|GetForwardVector CameraTrace))
  (bind _character (Variables|Default|GetCharacter))
  (bind _character_2 (Variables|Default|GetCharacter))
  (bind _returnvalue_3 (Math|Vector|GetForwardVector CameraTrace))
  (bind _mesh (Variables|/Script/Engine.Character|GetMesh _character_2))
  (bind _lockonwidget (Variables|/Game/DATA/BP_PC.BP_PC_C|GetLockOnWidget _character))
  (bind _returnvalue_4 (Transformation|GetWorldLocation _lockonwidget))
  (bind _returnvalue_5 (Class|SkinnedMeshComponent|GetSocketBoneName _mesh InSocketName))
  (bind _returnvalue_6 (Transformation|GetSocketLocation _mesh _returnvalue_5))
  (bind (_outhit _returnvalue_7) (Collision|SphereTraceForObjects (select (Variables|Default|GetIsPlayer) (+ (* (Math|Vector|Normalize _returnvalue_2) 3.1e+02) _returnvalue) (+ (* (Math|Vector|Normalize _returnvalue_3) 3.1e+02) _returnvalue_4)) (select (Variables|Default|GetIsPlayer) (+ _returnvalue (* _returnvalue_2 TraceRange)) (+ (+ _returnvalue_4 (* _returnvalue_3 TraceRange)) "0.000000,0.000000,200.000000")) Radius (Utilities|Array|MakeArray "ObjectTypeQuery1" "ObjectTypeQuery9" "ObjectTypeQuery8" "ObjectTypeQuery4" "ObjectTypeQuery6" "ObjectTypeQuery1") false ActorsToIgnore DrawDebugType))
  (bind (_outhit_2 _returnvalue_8) (Collision|SphereTraceForObjects (select SocketType _returnvalue_6 (select (Variables|Default|GetIsPlayer) (Transformation|GetWorldLocation CastLocTrace) (Transformation|GetWorldLocation (Variables|/Game/DATA/BP_PC.BP_PC_C|GetLockOnWidget (Variables|Default|GetCharacter))))) (Math|Vector|SelectVector (.impactpoint _outhit) (.traceend _outhit) _returnvalue_7) Radius (Utilities|Array|MakeArray "ObjectTypeQuery1" "ObjectTypeQuery9" "ObjectTypeQuery8" "ObjectTypeQuery4" "ObjectTypeQuery6") false ActorsToIgnore DrawDebugType))
  (return (Math|Transform|MakeTransform (Math|Vector|SelectVector (.impactpoint _outhit_2) (.traceend _outhit_2) _returnvalue_8) (Math|Rotator|FindLookatRotation (select SocketType _returnvalue_6 (Transformation|GetWorldLocation CastLocTrace)) (Math|Vector|SelectVector (.impactpoint _outhit_2) (.traceend _outhit_2) _returnvalue_8))) (select _returnvalue_8 true (select _returnvalue_7 true false))))

(fn Decal
  (params (HitInfo :type Hit%20Result%20Structure))
  (if (not (== (.HitActor (Collision|BreakHitResult HitInfo)) "/Game/DATA/Blueprints/Decals/BP_LightningDecal.BP_LightningDecal"))
    (CallFunction|SpawnDecal HitInfo "/Game/DATA/Blueprints/Decals/BP_LightningDecal.BP_LightningDecal_C" (* (Variables|Default|GetAreaEffect) 4.0) false "1.000000,1.000000,1.000000")))