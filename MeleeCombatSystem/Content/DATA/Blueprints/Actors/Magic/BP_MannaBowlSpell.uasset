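; Mana bowl spell actor that faces its character on spawn and grants a random heal or mana restore to a player entering its area.
; The overlap picks either effect at even odds, healing via negative damage scaled by a character substat, then plays effects and destroys itself.
; Untouched bowls expire after a random delay; both endings notify the spawner.
; A looping facing-checked Heal trace exists but nothing live calls it.
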(event OnComponentBeginOverlap(AreaOfEffect)
  (params (OverlappedComponent :type Primitive%20Component%20Object%20Reference) (OtherActor :type Actor%20Object%20Reference) (OtherComp :type Primitive%20Component%20Object%20Reference) (OtherBodyIndex :type Integer) (bFromSweep :type Boolean) (SweepResult :type Hit%20Result%20Structure%20%28by%20ref%29))
  (bind _asbp_pc (Utilities|Casting|CastToBP_PC OtherActor))
  (Utilities|FlowControl|Sequence
    (:then_0
      (Variables|Default|SetHealPower (* (Math|Random|RandomFloatinRange 1.0 (Default|GetSubStats (Variables|/Game/DATA/BP_PC.BP_PC_C|GetStatsComponent (Variables|Default|GetCharacter)) "NewEnumerator12")) -1.0))
      (if (> (Math|Random|RandomFloatinRange 1.0 1e+02) 5e+01)
        (CallFunction|ApplyDamage _asbp_pc SweepResult false 1.0)
        (Effects|SpawnEmitteratLocation "/Game/InfinityBladeEffects/Effects/FX_Ability/Heal/P_Health_Player_Buff_Ping_01.P_Health_Player_Buff_Ping_01" (.location (Transformation|GetActorTransform _asbp_pc)) (.rotation (Transformation|GetActorTransform _asbp_pc)) (.scale (Transformation|GetActorTransform _asbp_pc)))
        (Audio|PlaySoundatLocation "/Game/DATA/SoundFX/SC_Heal.SC_Heal" (Transformation|GetActorLocation _asbp_pc) "0, 0, 0" 1.0 1.0 0.0 0 0 0 0)
        (Actor|DestroyActor)
        (else
          (Default|ModifyCurrentStatValue (Variables|/Game/DATA/BP_PC.BP_PC_C|GetStatsComponent _asbp_pc) "NewEnumerator4" (* (Variables|Default|GetHealPower) -1.0) true)
          (bind _returnvalue (Niagara|SpawnSystemAttached "/Game/DATA/Effects/N_MagicPotionBurst.N_MagicPotionBurst" (Variables|/Script/Engine.Character|GetMesh _asbp_pc) "None" (Transformation|GetActorLocation _asbp_pc) "0, 0, 0" "KeepWorldPosition" true))
          (Class|NiagaraComponent|SetVariableInt _returnvalue "SpawnBurst" (Math|Float|Truncate (* (* (Variables|Default|GetHealPower) -1.0) 5.0)))
          (Audio|PlaySoundatLocation "/Game/DATA/SoundFX/SC_Heal_Mana.SC_Heal_Mana" (Transformation|GetActorLocation _asbp_pc) "0, 0, 0" 1.0 1.0 0.0 0 0 0 0)
          (Actor|DestroyActor))))
    (:then_1
      (Utilities|IsValid (Variables|Default|GetSpawner)
        (:Is%20Valid
          (Class|CombatBPI|ArtifactSpellDone(Message) (Variables|Default|GetSpawner)))))))

(event Custom|Heal
  (bind _mannabowl (Variables|Default|GetMannaBowl))
  (bind _returnvalue (Transformation|GetWorldLocation _mannabowl))
  (Utilities|FlowControl|Delay (Math|Random|RandomFloatinRange 1.0 5.0))
  (Variables|Default|SetHealPower (* (Math|Random|RandomFloatinRange 1.0 (Default|GetSubStats (Variables|/Game/DATA/BP_PC.BP_PC_C|GetStatsComponent (Variables|Default|GetCharacter)) "NewEnumerator12")) -1.0))
  (bind _outhits (Collision|MultiSphereTraceForObjects _returnvalue _returnvalue (Variables|Default|GetAreaEffect) (Utilities|Array|MakeArray "ObjectTypeQuery3") false 0 "None"))
  (bind _array_element (Utilities|Array|ForEachLoopwithBreak _outhits)
    (:LoopBody
      (if (> (Math|Vector|DotProduct (Transformation|GetActorForwardVector (.HitActor (Collision|BreakHitResult _array_element))) (Math|Vector|Normalize (- (Transformation|GetActorLocation) (Transformation|GetActorLocation (.HitActor (Collision|BreakHitResult _array_element)))))) 0.75)
        (CallFunction|ApplyDamage (Variables|Default|GetCharacter) _array_element false 1.0)
        (Effects|SpawnEmitteratLocation "/Game/InfinityBladeEffects/Effects/FX_Ability/Heal/P_Health_Player_Buff_Ping_01.P_Health_Player_Buff_Ping_01" (.location (Transformation|GetActorTransform (.HitActor (Collision|BreakHitResult _array_element)))) (.rotation (Transformation|GetActorTransform (.HitActor (Collision|BreakHitResult _array_element)))) (.scale (Transformation|GetActorTransform (.HitActor (Collision|BreakHitResult _array_element)))))
        (Audio|PlaySoundatLocation "/Game/DATA/SoundFX/SC_Heal.SC_Heal" (Transformation|GetActorLocation (.HitActor (Collision|BreakHitResult _array_element))) "0, 0, 0" 1.0 1.0 0.0 0 0 0 0)))
    (:Completed
      (CallFunction|Heal))))

(event Custom|Break
  (Utilities|Array|ForEachLoopwithBreak (stale Custom|Heal _outhits)) ; enters at Break
)

(event EventBeginPlay
  (bind _spawner (Variables|Default|GetSpawner))
  (|CallParentFunction)
  (Transformation|SetWorldRotation (Variables|Default|GetMannaBowl) (Math|Rotator|MakeRotator 0.0 0.0 (.yaw (Math|Rotator|FindLookatRotation (Transformation|GetActorLocation) (Transformation|GetActorLocation (Variables|Default|GetCharacter))))) false false)
  (Utilities|FlowControl|Delay (Math|Random|RandomFloatinRange 1e+01 25.0))
  (Utilities|IsValid _spawner
    (:Is%20Valid
      (Class|CombatBPI|ArtifactSpellDone(Message) _spawner))
    (:Is%20Not%20Valid
      _))
  (Actor|DestroyActor))

(event Collision|EventActorBeginOverlap
  (params (OtherActor :type Actor%20Object%20Reference)))

(event EventTick
  (params (DeltaSeconds :type Float%20%28single-precision%29))
  (|CallParentFunction DeltaSeconds) ; This node is disabled and will not be called.\nDrag off pins to build functionality.
)

(fn ConstructionScript
  (|CallParentFunction))