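; Fire stream spell actor that damages actors caught in a cone, deactivates after two seconds and destroys itself six seconds later.
; While active, the cone grows from zero to its original scale, and the trail's particle count, rate and flame size follow ParticleScale.
; New overlaps take a hit with sound; after a short delay the hit list clears and everything still inside is hit again.
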(event OnComponentBeginOverlap(Cone)
  (params (OverlappedComponent :type Primitive%20Component%20Object%20Reference) (OtherActor :type Actor%20Object%20Reference) (OtherComp :type Primitive%20Component%20Object%20Reference) (OtherBodyIndex :type Integer) (bFromSweep :type Boolean) (SweepResult :type Hit%20Result%20Structure%20%28by%20ref%29))
  (if (Variables|Default|GetActive)
    (if (not (Utilities|Array|ContainsItem (Variables|Default|GetActorsHit) OtherActor))
      (Utilities|Array|Add (Variables|Default|GetActorsHit) OtherActor)
      (Variables|Default|SetHitInfo SweepResult)
      (Variables|Default|SetHitActor OtherActor)
      (CallFunction|Hit)
      (Utilities|FlowControl|Delay 0.7)
      (Utilities|Array|Clear (Variables|Default|GetActorsHit))
      (for _array_element (Collision|GetOverlappingActors (Variables|Default|GetCone) 0 :!class /Script/Engine.PrimitiveComponent)
        (CallFunction|ApplyDamage _array_element (Variables|Default|GetHitInfo) true 1.0)
        (Audio|SpawnSoundatLocation "/Game/DATA/SoundFX/Fire/SC_AirSuck.SC_AirSuck" (Transformation|GetActorLocation _array_element) "0, 0, 0" 1.0 1.0 0.0 0 0)))))

(event EventBeginPlay
  (|CallParentFunction)
  (Utilities|FlowControl|Delay 2.0)
  (Variables|Default|SetActive false)
  (Transformation|SetWorldScale3D (Variables|Default|GetCone) "0, 0, 0")
  (Utilities|FlowControl|Delay 6.0)
  (Actor|DestroyActor))

(event Collision|EventActorBeginOverlap
  (params (OtherActor :type Actor%20Object%20Reference)))

(event EventTick
  (params (DeltaSeconds :type Float%20%28single-precision%29))
  (bind _trail (Variables|Default|GetTrail))
  (bind _particlescale (Variables|Default|GetParticleScale))
  (bind _particlescale_2 (Variables|Default|GetParticleScale))
  (bind _returnvalue (* 6e+02 _particlescale))
  (bind _returnvalue_2 (* 1e+03 _particlescale_2))
  (bind _returnvalue_3 (Math|Float|Truncate _returnvalue_2))
  (|CallParentFunction DeltaSeconds)
  (if (Variables|Default|GetActive)
    (Utilities|FlowControl|Sequence
      (:then_0
        (Utilities|FlowControl|DoOnce false
          (:Completed
            (Variables|Default|SetBoxSize (Transformation|GetWorldScale (Variables|Default|GetCone)))
            (Transformation|SetWorldScale3D (Variables|Default|GetCone) "0, 0, 0")
            (Effects|Components|ParticleSystem|SetFloatParameter (Variables|Default|GetTrail) "SpawnRate" (Math|Float|Clamp(Float) _returnvalue _returnvalue 2.4e+03))
            (Effects|Components|ParticleSystem|SetFloatParameter _trail "FlameSize" (* 0.5 (Variables|Default|GetParticleScale)))
            (Effects|Components|ParticleSystem|SetIntParameter _trail "Spawn Count" (Math|Integer|Clamp(Integer) _returnvalue_3 _returnvalue_3 4000)))))
      (:then_1
        (Transformation|SetWorldScale3D (Variables|Default|GetCone) (Math|Interpolation|VInterptoConstant (Transformation|GetWorldScale (Variables|Default|GetCone)) (Variables|Default|GetBoxSize) (Utilities|Time|GetWorldDeltaSeconds) 2e+01))))))

(event EventHit
  (CallFunction|ApplyDamage (Variables|Default|GetHitActor) (Variables|Default|GetHitInfo) true 1.0)
  (Audio|SpawnSoundatLocation "/Game/DATA/SoundFX/Fire/SC_AirSuck.SC_AirSuck" (Transformation|GetActorLocation (Variables|Default|GetHitActor)) "0, 0, 0" 1.0 1.0 0.0 0 0))

(fn ConstructionScript)