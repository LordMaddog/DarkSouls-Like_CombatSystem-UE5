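; Chain lightning spell actor that strikes a target with a Niagara beam, then arcs onward, living one second per link.
; Tick pins the beam between the previous target or start point and the current target, triggering throttled sphere-trace hits that place decals and accumulate damage.
; The first damaging hit searches nearby for another damageable actor and spawns a copy of itself toward it, with area effect shrinking each link.
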(event Custom|OnHit
  (params (LOC :type Vector))
  ;[1 1 1] Damage And Decal
  (bind _outhits (Collision|MultiSphereTraceForObjects LOC LOC (* (Variables|Default|GetAreaEffect) 6.0) (Utilities|Array|MakeArray "ObjectTypeQuery1" "ObjectTypeQuery4" "ObjectTypeQuery9" "ObjectTypeQuery6" "ObjectTypeQuery8" "ObjectTypeQuery5") false (Utilities|Array|MakeArray (Variables|Default|GetCharacter) self) "None"))
  (for _array_element _outhits
    (if (.bBlockingHit (Collision|BreakHitResult _array_element))
      (CallFunction|Decal _array_element)
      (bind _output_get (Variables|Default|SetDamageTemp (+ (* (Variables|Default|GetDamageOut) 0.3) (Variables|Default|GetDamageTemp))))
      (if (>= _output_get (Variables|Default|GetDamageOut))
        (Utilities|FlowControl|DoOnce false :!label _label
          (:Completed
            (Utilities|FlowControl|Sequence
              (:then_0
                (if (== (Variables|Default|GetTarget) (.HitActor (Collision|BreakHitResult _array_element)))
                  (CallFunction|ApplyDamage (Variables|Default|GetTarget) _array_element true 0.3)
                  (Variables|Default|SetDamageTemp 0.0)
                  (Utilities|FlowControl|DoOnce false
                    (:Completed
                      (Variables|Default|SetHitTarget (Variables|Default|GetTarget))
                      (Variables|Default|SetSpawnedChain 0)
                      (CallFunction|Chain LOC)))))
              (:then_1
                (Utilities|FlowControl|Delay 0.2)
                (goto _label Reset)))))))))

(event Custom|Chain
  (params (LOC :type Vector))
  ;[1 1 1] Chain
  (if (not (Utilities|IsValid (Variables|Default|GetSpawnedChain)))
    (bind _outhits (Collision|MultiSphereTraceForObjects LOC LOC (* (Variables|Default|GetAreaEffect) 1e+02) (Utilities|Array|MakeArray "ObjectTypeQuery1" "ObjectTypeQuery4" "ObjectTypeQuery9" "ObjectTypeQuery6" "ObjectTypeQuery8" "ObjectTypeQuery5") false (Utilities|Array|MakeArray (Variables|Default|GetCharacter) self (Variables|Default|GetStartedTarget) (Variables|Default|GetTarget)) "None"))
    (for _array_element _outhits
      (if (and (.bBlockingHit (Collision|BreakHitResult _array_element)) (not (Utilities|IsValid (Variables|Default|GetSpawnedChain))))
        (Utilities|IsValid (Actor|GetComponentbyClass (.HitActor (Collision|BreakHitResult _array_element)) "/Game/DATA/Blueprints/Components/CombatComponent.CombatComponent_C")
          (:Is%20Valid
            (bind _returnvalue (Default|CanReciveDamage (Actor|GetComponentbyClass (.HitActor (Collision|BreakHitResult _array_element)) "/Game/DATA/Blueprints/Components/CombatComponent.CombatComponent_C")))
            (if _returnvalue
              (if (not (== (Variables|Default|GetTarget) (.HitActor (Collision|BreakHitResult _array_element)))) :!label _label
                (Variables|Default|GetChainTarget
                  (:then
                    (if (< (Transformation|GetDistanceTo (.HitActor (Collision|BreakHitResult _array_element)) (Variables|Default|GetChainTarget)) (Variables|Default|GetDisttanceToCHainTarget))
                      (Variables|Default|SetDisttanceToCHainTarget (Transformation|GetDistanceTo (.HitActor (Collision|BreakHitResult _array_element)) (Variables|Default|GetChainTarget)) :!label _label_2)
                      (Variables|Default|SetChainTarget (.HitActor (Collision|BreakHitResult _array_element)))))
                  (:else
                    (goto _label_2))))))
          (:Is%20Not%20Valid
            (Utilities|IsValid (Actor|GetComponentbyClass (.HitActor (Collision|BreakHitResult _array_element)) "/Game/DATA/Blueprints/Components/inanimateObjectStats.inanimateObjectStats_C")
              (:Is%20Valid
                (bind _returnvalue_2 (Default|CanReciveDamage (Actor|GetComponentbyClass (.HitActor (Collision|BreakHitResult _array_element)) "/Game/DATA/Blueprints/Components/inanimateObjectStats.inanimateObjectStats_C")))
                (if _returnvalue_2
                  (goto _label))))))))
    (Variables|Default|GetChainTarget
      (:then
        (CallFunction|Spawn "0, 0, 0"))
      (:else))))

(event Custom|Spawn
  (params (StarLoc :type Vector))
  (bind _character (Variables|Default|GetCharacter))
  ;[1 1 1] Spawn
  (if (not (Utilities|IsValid (Variables|Default|GetSpawnedChain)))
    (Game|SpawnActorfromClass "BP_lightningChainSpell_C" (Math|Transform|MakeTransform (Transformation|GetActorLocation (Variables|Default|GetTarget)) "0, 0, 0" "1.000000,1.000000,1.000000") "Undefined" "MultiplyWithRoot" _character (Variables|Default|GetChainTarget) (Transformation|GetActorLocation (Variables|Default|GetHitTarget)) (Variables|Default|GetHitTarget) (Variables|Default|GetDamageMultiplier) (* (Variables|Default|GetAreaEffect) 0.8) 9e+02 0.0 _character (Variables|Default|GetBasePoiseDamgeMultiplier) false "(TagName=\"Character.Action.Skill/Magic.Lightning\")" false 0.0 _character)
    (Variables|Default|SetSpawnedChain 0)))

(event EventBeginPlay
  ;[1 1 1] Event Begin Play
  (|CallParentFunction)
  (Components|Activation|Activate (Variables|Default|GetTrail) false)
  (Effects|Components|ParticleSystem|SetFloatParameter (Variables|Default|GetTrail) "Scale" (Variables|Default|GetAreaEffect))
  (Audio|Components|Audio|SetVolumeMultiplier (Variables|Default|GetFlySound) (Variables|Default|GetAreaEffect) :!class /Script/Engine.AudioComponent)
  (Utilities|FlowControl|Delay 1.0)
  (Actor|DestroyActor))

(event EventTick
  (params (DeltaSeconds :type Float%20%28single-precision%29))
  (bind _target (Variables|Default|GetTarget))
  (bind _returnvalue (CallFunction|TargetExtentType _target))
  ;[1 1 1] Event Tick (sets beam start and end point)
  (Variables|Default|GetTrail
    (:then
      (Variables|Default|GetStartedTarget
        (:then
          (Transformation|SetWorldLocation (Variables|Default|GetMainProjectileCore) (CallFunction|TargetExtentType (Variables|Default|GetStartedTarget)) false true))
        (:else
          (Transformation|SetWorldLocation (Variables|Default|GetMainProjectileCore) (Variables|Default|GetStarLoc) false true)))
      (Utilities|FlowControl|Sequence
        (:then_0
          (Variables|Default|GetTrail
            (:then
              (Niagara|SetNiagaraVariable(Vector3) (Variables|Default|GetTrail) "Beam End" _returnvalue)
              (Utilities|FlowControl|Delay 0.2)
              (CallFunction|ActivateonOFF true (Variables|Default|GetTrail)))
            (:else)))
        (:then_1
          (Utilities|FlowControl|DoOnce false :!label _label
            (:Completed
              (CallFunction|OnHit _returnvalue)
              (Utilities|FlowControl|Delay 0.3)
              (goto _label Reset))))))
    (:else)))

(fn ConstructionScript
  (|CallParentFunction))

(fn ActivateonOFF
  (params (On :type Boolean) (Target :type Actor%20Component%20Object%20Reference))
  (if On
    (if (not (Components|Activation|IsActive Target))
      (Components|Activation|SetActive Target true false))
    (elif (Components|Activation|IsActive Target)
      (Components|Activation|SetActive Target false false))))

(fn GetAimTrace
  (params (CameraTrace :type Scene%20Component%20Object%20Reference) (CastLocTrace :type Scene%20Component%20Object%20Reference) (TraceRange :type Float%20%28single-precision%29) (Radius :type Float%20%28single-precision%29) (DrawDebugType :type EDrawDebugTrace%20Enum :default "None") (SocketType :type Boolean) (InSocketName :type Name) (ActorsToIgnore :type Array%20of%20Actor%20Object%20References))
  (bind _returnvalue (Transformation|GetWorldLocation CameraTrace))
  (bind _returnvalue_2 (Math|Vector|GetForwardVector CameraTrace))
  (bind _character (Variables|Default|GetCharacter))
  (bind _character_2 (Variables|Default|GetCharacter))
  (bind _returnvalue_3 (Math|Vector|GetForwardVector CameraTrace))
  (bind _mesh (Variables|/Script/Engine.Character|GetMesh _character_2))
  (bind _lockonwidget (Variables|/Game/DATA/BP_PC.BP_PC_C|GetLockOnWidget _character))
  (bind _returnvalue_4 (Transformation|GetWorldLocation _lockonwidget))
  (bind _returnvalue_5 (Class|SkinnedMeshComponent|GetSocketBoneName _mesh InSocketName))
  (bind _returnvalue_6 (Transformation|GetSocketLocation _mesh _returnvalue_5))
  (bind (_outhit _returnvalue_7) (Collision|SphereTraceForObjects (select (Variables|Default|GetIsPlayer) (+ (* (Math|Vector|Normalize _returnvalue_2) 3.1e+02) _returnvalue) (+ (* (Math|Vector|Normalize _returnvalue_3) 3.1e+02) _returnvalue_4)) (select (Variables|Default|GetIsPlayer) (+ _returnvalue (* _returnvalue_2 TraceRange)) (+ (+ _returnvalue_4 (* _returnvalue_3 TraceRange)) "0.000000,0.000000,200.000000")) Radius (Utilities|Array|MakeArray "ObjectTypeQuery1" "ObjectTypeQuery9" "ObjectTypeQuery8" "ObjectTypeQuery4" "ObjectTypeQuery6" "ObjectTypeQuery1") false ActorsToIgnore DrawDebugType))
  (bind (_outhit_2 _returnvalue_8) (Collision|SphereTraceForObjects (select SocketType _returnvalue_6 (select (Variables|Default|GetIsPlayer) (Transformation|GetWorldLocation CastLocTrace) (Transformation|GetWorldLocation (Variables|/Game/DATA/BP_PC.BP_PC_C|GetLockOnWidget (Variables|Default|GetCharacter))))) (Math|Vector|SelectVector (.impactpoint _outhit) (.traceend _outhit) _returnvalue_7) Radius (Utilities|Array|MakeArray "ObjectTypeQuery1" "ObjectTypeQuery9" "ObjectTypeQuery8" "ObjectTypeQuery4" "ObjectTypeQuery6") false ActorsToIgnore DrawDebugType))
  (return (Math|Transform|MakeTransform (Math|Vector|SelectVector (.impactpoint _outhit_2) (.traceend _outhit_2) _returnvalue_8) (Math|Rotator|FindLookatRotation (select SocketType _returnvalue_6 (Transformation|GetWorldLocation CastLocTrace)) (Math|Vector|SelectVector (.impactpoint _outhit_2) (.traceend _outhit_2) _returnvalue_8))) (select _returnvalue_8 true (select _returnvalue_7 true false))))

(fn TargetExtentType
  (params (Target :type Actor%20Object%20Reference))
  (Utilities|IsValid Target
    (:Is%20Valid
      (return (select (.bSuccess (Utilities|Casting|CastToBP_PC Target)) (Transformation|GetActorLocation Target) (.Origin (Collision|GetActorBounds Target false false)))))))

(fn Decal
  (params (HitInfo :type Hit%20Result%20Structure))
  (if (not (== (.HitActor (Collision|BreakHitResult HitInfo)) "/Game/DATA/Blueprints/Decals/BP_LightningDecal.BP_LightningDecal"))
    (CallFunction|SpawnDecal HitInfo "/Game/DATA/Blueprints/Decals/BP_LightningDecal.BP_LightningDecal_C" (* (Variables|Default|GetAreaEffect) 4.0) false "1.000000,1.000000,1.000000")))