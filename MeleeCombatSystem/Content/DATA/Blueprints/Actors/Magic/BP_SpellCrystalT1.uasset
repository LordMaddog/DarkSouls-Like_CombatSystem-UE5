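; Tier 1 crystal spell projectile that damages what it hits, then sticks to it and shrinks away, or explodes.
; Construction scales the crystal and blast sphere from DamageOut.
; On hit it attaches to the character's bone or the actor, swaps collision, and Tick shrinks mesh and radius until destruction.
; Explosion damages everything overlapping the sphere, triggered by an impact flag, hitting another spell, or taking sufficient damage.
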(event Custom|ExplodOnImpact!
  ;[1 1 1] Explode when damaged.
  (for _array_element (Collision|GetOverlappingActors (Variables|Default|GetAreaOfEffect) 0 :!class /Script/Engine.PrimitiveComponent)
    (CallFunction|ApplyDamage _array_element (Variables|Default|GetHitInfo) true 1.0))
  (Components|Activation|Activate (Variables|Default|GetP_Buff) true)
  (Utilities|FlowControl|Delay 1.0)
  (Actor|DestroyActor))

(event EventBeginPlay
  (|CallParentFunction) ; This node is disabled and will not be called.\nDrag off pins to build functionality.
)

(event Collision|EventActorBeginOverlap
  (params (OtherActor :type Actor%20Object%20Reference)))

(event Game|Damage|EventAnyDamage
  (params (Damage :type Float%20%28single-precision%29) (DamageType :type Damage%20Type%20Object%20Reference) (InstigatedBy :type Controller%20Object%20Reference) (DamageCauser :type Actor%20Object%20Reference))
  ;[1 1 1] Explode when damaged.
  (if (>= Damage 3.0)
    (Utilities|FlowControl|DoOnce false
      (:Completed
        (for _array_element (Collision|GetOverlappingActors (Variables|Default|GetAreaOfEffect) 0 :!class /Script/Engine.PrimitiveComponent)
          (CallFunction|ApplyDamage _array_element (Variables|Default|GetHitInfo) true 1.0))
        (Components|Activation|Activate (Variables|Default|GetP_Buff) true)
        (Utilities|FlowControl|Delay 1.0)
        (Actor|DestroyActor)))))

(event EventTick
  (params (DeltaSeconds :type Float%20%28single-precision%29))
  ;[1 1 1] Strink
  (if (Variables|Default|GetStartShrink)
    (Transformation|SetWorldScale3D (Variables|Default|GetVisualEffect) (Math|Conversions|ToVector(Float) (Math|Interpolation|FInterptoConstant (.x (Transformation|GetWorldScale (Variables|Default|GetVisualEffect))) 0.0 (Utilities|Time|GetWorldDeltaSeconds) 0.02)))
    (Components|Sphere|SetSphereRadius (Variables|Default|GetAreaOfEffect) (Math|Interpolation|FInterptoConstant (Variables|/Script/Engine.SphereComponent|GetSphereRadius (Variables|Default|GetAreaOfEffect)) 0.0 (Utilities|Time|GetWorldDeltaSeconds) 1.0) false)
    (if (== (.x (Transformation|GetWorldScale (Variables|Default|GetVisualEffect))) 0.0)
      _
      (else
        (Utilities|FlowControl|Delay 1.0)
        (Utilities|IsValid (Variables|Default|GetHitActor)
          (:Is%20Not%20Valid
            _))))
    (Actor|DestroyActor)))

(event EventHit
  (bind _hitactor (Variables|Default|GetHitActor))
  ;[1 1 1] Hit
  (|CallParentFunction)
  (Utilities|FlowControl|DoOnce false
    (:Completed
      (Niagara|SetNiagaraVariable(Float) (Variables|Default|GetN_Ice_Trail) "Spawn Spacing" 0.0)
      (Components|Activation|Activate (Variables|Default|GetImpactSound) true)
      (Audio|Components|Audio|Stop (Variables|Default|GetFlySound))
      (CallFunction|ApplyDamage (Variables|Default|GetHitActor) (Variables|Default|GetHitInfo) false 1.0)
      (if (not (Variables|Default|GetExplodOnImpact))
        (bind _ascharacter (Utilities|Casting|CastToCharacter (Variables|Default|GetHitActor))
          (:then
            (Transformation|AttachComponentToComponent (Variables|Default|GetMainProjectileCore) (Variables|/Script/Engine.Character|GetMesh _ascharacter) (.HitBoneName (Collision|BreakHitResult (Variables|Default|GetHitInfo))) "KeepWorld" "KeepWorld" "KeepWorld" true)
            (Collision|SetCollisionResponsetoChannel (Variables|Default|GetVisualEffect) "ECC_Pawn" "ECR_Ignore")
            (Collision|SetCollisionResponsetoChannel (Variables|Default|GetVisualEffect) "ECC_Visibility" "ECR_Ignore")
            (Collision|SetCollisionResponsetoChannel (Variables|Default|GetVisualEffect) "ECC_Camera" "ECR_Ignore")
            (Collision|SetCollisionResponsetoChannel (Variables|Default|GetVisualEffect) "ECC_GameTraceChannel2" "ECR_Block")
            (Variables|Default|SetStartShrink true :!label _label))
          (:CastFailed
            (Utilities|IsValid _hitactor
              (:Is%20Valid
                (Transformation|AttachActorToActor _hitactor "None" "KeepWorld" "KeepWorld" "KeepWorld" true)
                (Utilities|Casting|CastToBP_BaseSpell (Variables|Default|GetHitActor)
                  (:then
                    (CallFunction|ExplodonImpact!))
                  (:CastFailed
                    (Collision|SetCollisionObjectType (Variables|Default|GetVisualEffect) "ECC_WorldStatic")
                    (Collision|SetCollisionResponsetoChannel (Variables|Default|GetVisualEffect) "ECC_Pawn" "ECR_Block")
                    (Collision|SetCollisionEnabled (Variables|Default|GetVisualEffect) "QueryAndPhysics")
                    (Collision|SetCollisionEnabled (Variables|Default|GetMainProjectileCore) "NoCollision")
                    (Utilities|FlowControl|Delay 0.1)
                    (goto _label))))
              (:Is%20Not%20Valid
                (Actor|DestroyActor)))))
        (else
          (CallFunction|ExplodonImpact!))))))

(fn ConstructionScript
  (bind _damageout (Variables|Default|GetDamageOut))
  (bind _returnvalue (* _damageout 0.1))
  ;[1 1 1] Set size and area of effect
  (|CallParentFunction)
  (Transformation|SetWorldScale3D (Variables|Default|GetVisualEffect) (+ (Transformation|GetWorldScale (Variables|Default|GetVisualEffect)) (Math|Float|Clamp(Float) _returnvalue _returnvalue 9.0)))
  (Components|Sphere|SetSphereRadius (Variables|Default|GetAreaOfEffect) (+ (Variables|Default|GetAreaEffect) (Variables|Default|GetDamageOut)) true))