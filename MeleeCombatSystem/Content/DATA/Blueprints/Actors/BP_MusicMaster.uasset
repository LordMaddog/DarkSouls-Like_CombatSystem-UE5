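; Music manager actor that plays area and combat music from DT_Music, crossfading between two spawned 2D audio components.
; BeginPlay caches rows into a map, where playback positions are saved so songs resume.
; EnterArea switches area songs; EnterCombat picks combat tracks by index and priority; non-interruptible requests defer a queued song name.
; A timer purges invalid attackers, and once none remain, area music restarts, checking BP_MusicArea for changes.
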(event Custom|SecondaryPercentage
  (params (PlayingSoundWave :type Sound%20Wave%20Object%20Reference) (PlaybackPercent :type Float%20%28single-precision%29))
  ;[1 1 1] Update current combat Song Time
  (Variables|Default|SetCurrentCombatSongTime (* PlaybackPercent (Variables|/Script/Engine.SoundBase|GetDuration PlayingSoundWave))))

(event Custom|PrimarySoundDone
  (bind _currentsong (CallFunction|GetNextSong))
  (bind (_nameout _song _start_time _volume) (CallFunction|GetSong _currentsong))
  ;[1 1 1] Area Song over get new one
  (Variables|Default|SetCurrentSongTime 0.0)
  (CallFunction|SaveCurrentSongTime)
  (CallFunction|PlayMusic _nameout _song _start_time _volume 3.0)
  (Variables|Default|SetDelayedWantedSong "---"))

(event Custom|ExitCombat
  (params (NPCIn :type BP%20Master%20AI%20Object%20Reference%20%28by%20ref%29))
  ;[1 1 1] ExitCombat
  (CallFunction|RemoveAttacking NPCIn)
  (Utilities|FlowControl|RetriggerableDelay (Math|Random|RandomFloatinRange 3.0 15.0))
  (if (CallFunction|AllAttackersGone)
    (CallFunction|SaveCurrentCombatSongTime)
    (Variables|Default|SetInCombat false)
    (Variables|Default|SetCurrentCombatSong "---")
    (Audio|Components|Audio|FadeOut (Variables|Default|GetSoundSecondary) 6.0 0.0 "Linear" :!class /Script/Engine.AudioComponent)
    (CallFunction|RestartAreaMusic)
    (Utilities|Time|ClearandInvalidateTimerbyHandle (Variables|Default|GetCombatTimer))))

(event Custom|RestartAreaMusic
  (bind (_value _newsongname) (CallFunction|CheckifSongShouldChange))
  (bind _currentsong (Variables|Default|GetCurrentSong))
  (bind (_nameout _song _start_time _volume) (CallFunction|GetSong _currentsong))
  (bind (_nameout_2 _song_2 _start_time_2 _volume_2) (CallFunction|GetSong _newsongname))
  ;[1 1 1] After Combat End Restart Area Music
  (if (not _value)
    (CallFunction|PlayMusic _nameout _song _start_time _volume 6.0)
    (else
      (CallFunction|PlayMusic _nameout_2 _song_2 _start_time_2 _volume_2 6.0))))

(event Custom|StartCombatCheckTimer
  ;[1 1 1] Timer to check if still in combat
  (if (not (Utilities|Time|IsValidTimerHandle (Variables|Default|GetCombatTimer)))
    (bind _returnvalue (Utilities|Time|SetTimerbyFunctionName 0 "AreAttackersValid" 5.0 true))
    (Variables|Default|SetCombatTimer _returnvalue)))

(event Custom|SecondarySoundEnd
  ;[1 1 1] Loop Combat Song
  (Variables|Default|SetCurrentCombatSongTime 0.0)
  (CallFunction|SaveCurrentCombatSongTime)
  (if (Variables|Default|GetInCombat)
    (CallFunction|CombatPlaySong (.NameOut (CallFunction|GetSong (select (CallFunction|IsSongValid (Variables|Default|GetDelayedCombatSong)) (Variables|Default|GetDelayedCombatSong) (Variables|Default|GetCurrentCombatSong)))) (.Song (CallFunction|GetSong (select (CallFunction|IsSongValid (Variables|Default|GetDelayedCombatSong)) (Variables|Default|GetDelayedCombatSong) (Variables|Default|GetCurrentCombatSong)))) (.Start%20Time (CallFunction|GetSong (select (CallFunction|IsSongValid (Variables|Default|GetDelayedCombatSong)) (Variables|Default|GetDelayedCombatSong) (Variables|Default|GetCurrentCombatSong)))) (.Volume (CallFunction|GetSong (select (CallFunction|IsSongValid (Variables|Default|GetDelayedCombatSong)) (Variables|Default|GetDelayedCombatSong) (Variables|Default|GetCurrentCombatSong)))) 3.0)
    (Variables|Default|SetDelayedCombatSong "---")))

(event Custom|EnterArea
  (params (SongIn :type Name))
  ;[1 1 1] Change area song by changing areas
  (bind _output_get (Variables|Default|SetDesiredSong SongIn))
  (if (!= (Variables|Default|GetCurrentSong) _output_get)
    (CallFunction|SaveCurrentSongTime)
    (Audio|Components|Audio|FadeOut (Variables|Default|GetSoundPrimary) 2.0 0.0 "Linear" :!class /Script/Engine.AudioComponent)
    (Utilities|FlowControl|Delay 2.0)
    (CallFunction|PlayMusic (.NameOut (CallFunction|GetSong (Variables|Default|GetDesiredSong))) (.Song (CallFunction|GetSong (Variables|Default|GetDesiredSong))) (.Start%20Time (CallFunction|GetSong (Variables|Default|GetDesiredSong))) (.Volume (CallFunction|GetSong (Variables|Default|GetDesiredSong))) 2.0)))

(event Custom|CombatPlaySong
  (params (CurrentSong :type Name) (Song :type Sound%20Base%20Object%20Reference) (StartTime :type Float%20%28single-precision%29) (VolumeMultiplier :type Float%20%28single-precision%29) (FadeInDuration :type Float%20%28single-precision%29))
  (bind _soundsecondary (Variables|Default|GetSoundSecondary))
  ;[1 1 1] Play Combat Song
  (if (CallFunction|CanSongbeInterupted CurrentSong)
    (Variables|Default|SetCurrentCombatSong CurrentSong)
    (Audio|Components|Audio|SetSound _soundsecondary Song)
    (Audio|Components|Audio|Play _soundsecondary StartTime)
    (Audio|Components|Audio|SetVolumeMultiplier _soundsecondary VolumeMultiplier :!class /Script/Engine.AudioComponent)
    (Audio|Components|Audio|FadeIn _soundsecondary FadeInDuration 1.0 0.0 "Linear" :!class /Script/Engine.AudioComponent)
    (else
      (Variables|Default|SetDelayedCombatSong CurrentSong))))

(event Custom|PrimaryPercentage
  (params (PlayingSoundWave :type Sound%20Wave%20Object%20Reference) (PlaybackPercent :type Float%20%28single-precision%29))
  ;[1 1 1] Save song Time
  (Variables|Default|SetCurrentSongTime (* PlaybackPercent (Variables|/Script/Engine.SoundBase|GetDuration PlayingSoundWave))))

(event Custom|EnterCombat
  (params (NPCIn :type BP%20Master%20AI%20Object%20Reference%20%28by%20ref%29) (Index :type Integer))
  (bind (_songname _song _start_time _volume _change) (CallFunction|GetCombatSong Index))
  ;[1 1 1] Enter combat
  (if (CallFunction|NotAllreadyAttacking NPCIn)
    (Variables|Default|SetInCombat true)
    (if _change
      (CallFunction|CombatPlaySong _songname _song _start_time _volume 3.0)
      (CallFunction|SaveCurrentSongTime)
      (Audio|Components|Audio|FadeOut (Variables|Default|GetSoundPrimary) 3.0 0.0 "Linear" :!class /Script/Engine.AudioComponent)
      (CallFunction|StartCombatCheckTimer))))

(event Custom|PlayMusic
  (params (CurrentSong :type Name) (Song :type Sound%20Base%20Object%20Reference) (StartTime :type Float%20%28single-precision%29) (VolumeMultiplier :type Float%20%28single-precision%29) (FadeInDuration :type Float%20%28single-precision%29))
  (bind _soundprimary (Variables|Default|GetSoundPrimary))
  ;[1 1 1] Play default and area songs
  (if (CallFunction|CanSongbeInterupted CurrentSong)
    (if (not (Variables|Default|GetInCombat))
      (Variables|Default|SetCurrentSong CurrentSong)
      (Audio|Components|Audio|SetSound _soundprimary Song)
      (Audio|Components|Audio|Play _soundprimary StartTime)
      (Audio|Components|Audio|SetVolumeMultiplier _soundprimary VolumeMultiplier :!class /Script/Engine.AudioComponent)
      (Audio|Components|Audio|FadeIn _soundprimary FadeInDuration 1.0 0.0 "Linear" :!class /Script/Engine.AudioComponent))
    (else
      (Variables|Default|SetDelayedWantedSong CurrentSong))))

(event EventBeginPlay
  (bind _defaultsong (Variables|Default|GetDefaultSong))
  (bind (_nameout _song _start_time _volume) (CallFunction|GetSong _defaultsong))
  ;[1 1 1] Event begin play
  (CallFunction|SpawnSound)
  (bind _outrownames (DataTable|GetDataTableRowNames "/Game/DATA/Blueprints/DataTables/DT_Music.DT_Music"))
  (for (_array_element _array_index) _outrownames
    (CallFunction|SaveDefaultSong _array_element _array_index)
    (bind _returnvalue (Utilities|GetDataTableRow "/Game/DATA/Blueprints/DataTables/DT_Music.DT_Music" _array_element)
      (:then
        (Utilities|Map|Add (Variables|Default|GetSong) _array_element _returnvalue)
        (Utilities|FlowControl|Delay 1.0)
        (CallFunction|PlayMusic _nameout _song _start_time _volume 6.0)))))

(fn ConstructionScript)

(fn SaveDefaultSong
  (params (Song :type Name) (Index :type Integer))
  (if (== Index 0)
    (Variables|Default|SetDefaultSong Song)))

(fn GetSong
  (params (NameIn :type Name%20%28by%20ref%29))
  (bind _song (Variables|Default|GetSong))
  (bind _value (Utilities|Map|Find _song NameIn))
  (return NameIn (.song _value) (.starttime _value) (.volume _value)))

(fn SpawnSound
  (bind _returnvalue (Audio|SpawnSound2D "/Game/DATA/SoundFX/XP/Xp9.Xp9" 1.0 1.0 0.0 0 false false))
  (bind _output_get (Variables|Default|SetSoundPrimary _returnvalue))
  (Audio|Components|Audio|SetVolumeMultiplier _output_get 0.0 :!class /Script/Engine.AudioComponent)
  (EventDispatchers|BindEventtoOnAudioFinished _output_get (EventDispatchers|CreateEvent :!event Custom|PrimarySoundDone))
  (EventDispatchers|BindEventtoOnAudioPlaybackPercent (Variables|Default|GetSoundPrimary) (EventDispatchers|CreateEvent :!event Custom|PrimaryPercentage))
  (bind _returnvalue_2 (Audio|SpawnSound2D "/Game/DATA/SoundFX/XP/Xp9.Xp9" 1.0 1.0 0.0 0 false false))
  (bind _output_get_2 (Variables|Default|SetSoundSecondary _returnvalue_2))
  (Audio|Components|Audio|SetVolumeMultiplier _output_get_2 0.0 :!class /Script/Engine.AudioComponent)
  (EventDispatchers|BindEventtoOnAudioFinished (Variables|Default|GetSoundSecondary) (EventDispatchers|CreateEvent :!event Custom|SecondarySoundEnd))
  (EventDispatchers|BindEventtoOnAudioPlaybackPercent (Variables|Default|GetSoundSecondary) (EventDispatchers|CreateEvent :!event Custom|SecondaryPercentage)))

(fn GetNextSong
  (bind _l_songs (LocalVariables|GetL_Songs))
  (if (not (.ReturnValue (Utilities|Map|Find (Variables|Default|GetSong) (Variables|Default|GetDelayedWantedSong))))
    (if (.atendplayrandomsong (.Value (Utilities|Map|Find (Variables|Default|GetSong) (Variables|Default|GetCurrentSong))))
      (Utilities|Array|Clear (LocalVariables|GetL_Songs))
      (bind _keys (Utilities|Map|Keys (Variables|Default|GetSong)))
      (for _array_element _keys
        (if (.CanBePlayedAtRandom (Utilities|Struct|BreakS_Music (.Value (Utilities|Map|Find (Variables|Default|GetSong) _array_element))))
          (Utilities|Array|Add (LocalVariables|GetL_Songs) _array_element)))
      (return (Utilities|Array|Get(acopy) _l_songs (Math|Random|RandomIntegerinRange 0 (+ (Utilities|Array|Length _l_songs) 1))))
      (else
        (return (Variables|Default|GetCurrentSong))))
    (else
      (return (Variables|Default|GetDelayedWantedSong)))))

(fn SaveCurrentSongTime
  (bind _structout (Utilities|Struct|SetmembersinS_Music (.Value (Utilities|Map|Find (Variables|Default|GetSong) (Variables|Default|GetCurrentSong))) (Variables|Default|GetCurrentSongTime)))
  (Utilities|Map|Add (Variables|Default|GetSong) (Variables|Default|GetCurrentSong) _structout))

(fn NotAllreadyAttacking
  (params (NPCIN :type BP%20Master%20AI%20Object%20Reference%20%28by%20ref%29))
  (if (Utilities|Array|ContainsItem (Variables|Default|GetAttackingActors) NPCIN)
    (return false)
    (else
      (Utilities|Array|Add (Variables|Default|GetAttackingActors) NPCIN)
      (return true))))

(fn GetCombatSong
  (params (IndexIn :type Integer))
  (bind (_returnvalue _combatpriority) (CallFunction|GetSongIndex))
  (if (not _returnvalue)
    _
    (else
      (bind _output_get (LocalVariables|SetL_currentPriority _combatpriority))
      (if (< _output_get (.Combat%20Priority (CallFunction|GetCombatIndexPriority IndexIn)))
        _
        (else
          (return "None" 0 0.0 0.0 false)))))
  (bind _keys (Utilities|Map|Keys (Variables|Default|GetSong)))
  (for _array_element _keys
    (if (== (.combatindex (.Value (Utilities|Map|Find (Variables|Default|GetSong) _array_element))) IndexIn)
      (return _array_element (.song (.Value (Utilities|Map|Find (Variables|Default|GetSong) _array_element))) (.starttime (.Value (Utilities|Map|Find (Variables|Default|GetSong) _array_element))) (.volume (.Value (Utilities|Map|Find (Variables|Default|GetSong) _array_element))) true)))
  (bind _keys_2 (Utilities|Map|Keys (Variables|Default|GetSong)))
  (for _array_element_2 _keys_2
    (if (.iscombatsong (.Value (Utilities|Map|Find (Variables|Default|GetSong) _array_element_2)))
      (return _array_element_2 (.song (.Value (Utilities|Map|Find (Variables|Default|GetSong) _array_element_2))) (.starttime (.Value (Utilities|Map|Find (Variables|Default|GetSong) _array_element_2))) (.volume (.Value (Utilities|Map|Find (Variables|Default|GetSong) _array_element_2))) true))))

(fn RemoveAttacking
  (params (NPCIn :type BP%20Master%20AI%20Object%20Reference%20%28by%20ref%29))
  (if (Utilities|Array|ContainsItem (Variables|Default|GetAttackingActors) NPCIn)
    (Utilities|Array|RemoveItem (Variables|Default|GetAttackingActors) NPCIn)))

(fn GetCombatIndexPriority
  (params (IndexIn :type Integer))
  (bind _keys (Utilities|Map|Keys (Variables|Default|GetSong)))
  (for _array_element _keys
    (if (.iscombatsong (.Value (Utilities|Map|Find (Variables|Default|GetSong) _array_element)))
      (if (== (.combatindex (.Value (Utilities|Map|Find (Variables|Default|GetSong) _array_element))) IndexIn)
        (return (.combatpriority (.Value (Utilities|Map|Find (Variables|Default|GetSong) _array_element))) true))))
  (return 0 false))

(fn GetSongIndex
  (bind _song (Variables|Default|GetSong))
  (bind _currentcombatsong (Variables|Default|GetCurrentCombatSong))
  (bind (_value _returnvalue) (Utilities|Map|Find _song _currentcombatsong))
  (return _returnvalue (.CombatPriority (Utilities|Struct|BreakS_Music _value))))

(fn SaveCurrentCombatSongTime
  (bind _structout (Utilities|Struct|SetmembersinS_Music (.Value (Utilities|Map|Find (Variables|Default|GetSong) (Variables|Default|GetCurrentCombatSong))) (Variables|Default|GetCurrentCombatSongTime)))
  (Utilities|Map|Add (Variables|Default|GetSong) (Variables|Default|GetCurrentCombatSong) _structout))

(fn CheckifSongShouldChange
  (bind _outactors (Actor|GetAllActorsOfClass "/Game/DATA/Blueprints/Actors/BP_MusicArea.BP_MusicArea_C"))
  (for _array_element _outactors
    (bind (_output_get _data_table_row_name) (Default|CheckifPlayerin _array_element))
    (return _output_get _data_table_row_name)))

(fn AllAttackersGone
  (return (Utilities|Array|IsEmpty (Variables|Default|GetAttackingActors))))

(fn AreAttackersValid
  (Utilities|Array|Clear (LocalVariables|GetL_Invalid))
  (for _array_element (Variables|Default|GetAttackingActors)
    (Utilities|IsValid _array_element
      (:Is%20Not%20Valid
        (Utilities|Array|Add (LocalVariables|GetL_Invalid) _array_element))))
  (for _array_element_2 (LocalVariables|GetL_Invalid)
    (CallFunction|ExitCombat _array_element_2)))

(fn CanSongbeInterupted
  (params (Key :type Name%20%28by%20ref%29))
  (return (Utilities|Struct|BreakS_Music (.Value (Utilities|Map|Find (Variables|Default|GetSong) Key)))))

(fn IsSongValid
  (params (SongIn :type Name%20%28by%20ref%29))
  (return (.ReturnValue (Utilities|Map|Find (Variables|Default|GetSong) SongIn))))