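; Base actor for a magic bridge whose floor pieces assemble when the player enters its trigger box, with child hooks for part lists and special events.
; Pieces can start physics-collapsed, then timelines lerp them from saved fallen to original transforms in three random staggered groups.
; On exit they stay assembled, drop with physics or reverse magically, briefly relaxing collision on problem parts.
; Movement has optional sound and particles; impacts play surface-based effects.
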(event OnComponentBeginOverlap(Box)
  (params (OverlappedComponent :type Primitive%20Component%20Object%20Reference) (OtherActor :type Actor%20Object%20Reference) (OtherComp :type Primitive%20Component%20Object%20Reference) (OtherBodyIndex :type Integer) (bFromSweep :type Boolean) (SweepResult :type Hit%20Result%20Structure%20%28by%20ref%29))
  ;[1 1 1] Start
  (if (== (Game|GetPlayerCharacter 0) OtherActor)
    (Variables|Default|GetPlayer
      (:then
        _)
      (:else
        (bind _ascharacter (Utilities|Casting|CastToCharacter OtherActor))
        (Variables|Default|SetPlayer _ascharacter)))
    (Variables|Default|SetSilent false)
    (Variables|Default|SetActive true)
    (if (not (Variables|Default|GetStay%20Assembled))
      (if (Variables|Default|GetCan%20Assemble) :!label _label
        (Utilities|Time|ClearandInvalidateTimerbyHandle (Variables|Default|GetRemoveEffectsTimer))
        (for (_array_element _array_index) (Variables|Default|GetFloor)
          (Physics|SetSimulatePhysics _array_element false)
          (CallFunction|SpawnMovementEffects _array_element)
          (if (Variables|Default|GetMagicBack)
            _
            (else
              (Utilities|Map|Add (Variables|Default|GetFallenLoc&Rot) _array_index (Utilities|Struct|MakeS_VectorAndRotation (.location (Transformation|GetWorldTransform _array_element)) (.rotation (Transformation|GetWorldTransform _array_element))))))
          (if (not (Variables|Default|GetSet))
            (switch int (Math|Random|RandomIntegerinRange 0 2)
              (:0
                (Utilities|Array|Add (Variables|Default|GetArray1) _array_element))
              (:1
                (Utilities|Array|Add (Variables|Default|GetArray2) _array_element))
              (:2
                (Utilities|Array|Add (Variables|Default|GetArray3) _array_element)))))
        (Variables|Default|SetSet true)
        (CallFunction|MovementActivate))
      (elif (not (Variables|Default|GetAllready%20Assembled))
        (goto _label)))))

(event OnComponentEndOverlap(Box)
  (params (OverlappedComponent :type Primitive%20Component%20Object%20Reference) (OtherActor :type Actor%20Object%20Reference) (OtherComp :type Primitive%20Component%20Object%20Reference) (OtherBodyIndex :type Integer))
  ;[1 1 1] End
  (if (== OtherActor (Variables|Default|GetPlayer))
    (if (not (Variables|Default|GetStay%20Disassembled))
      _
      (else
        (Variables|Default|SetCan%20Assemble false)))
    (if (not (Variables|Default|GetStay%20Assembled))
      (Utilities|FlowControl|Sequence
        (:then_0
          (Utilities|ProblematicPartFix
            (:>
              (Variables|Default|SetActive false)
              (CallFunction|SpecialEventOff)
              (if (not (Variables|Default|GetMagicBack))
                (for _array_element (Variables|Default|GetFloor)
                  (Physics|SetSimulatePhysics _array_element true))
                (Utilities|FlowControl|RetriggerableDelay 1e+01)
                (CallFunction|EndSim)
                (else
                  (CallFunction|Reverse))))))
        (:then_1
          (if (Variables|Default|GetPeacfuly%20Disassemble)
            (Utilities|PeacefulDisassembly 2.0))))
      (else
        (CallFunction|StayAssembledEnd)))))

(event Custom|SetProblematicArray
  ;[1 1 1] Things Set on spawn
)

(event Custom|SetArray
  ;[1 1 1] Things Set on spawn
)

(event Custom|EndSim
  ;[1 1 1] End simulation (turns off simulation after a 10s delay)
  (for _array_element (Variables|Default|GetFloor)
    (Physics|SetSimulatePhysics _array_element false)))

(event Custom|SavePartsLocation
  ;[1 1 1] CustSaveStartLoc
  (for (_array_element _array_index) (Variables|Default|GetFloor)
    (Utilities|Map|Add (Variables|Default|GetFallenLoc&Rot) _array_index (Utilities|Struct|MakeS_VectorAndRotation (.location (Transformation|GetWorldTransform _array_element)) (.rotation (Transformation|GetWorldTransform _array_element)))))
  (CallFunction|SaveLoc))

(event Custom|Reverse
  ;[1 1 1] Move the bridge
  (CallFunction|ReactivateMovementEffects)
  (Utilities|Time|ClearandInvalidateTimerbyHandle (Variables|Default|GetRemoveEffectsTimer))
  (Variables|Default|SetReveresed true)
  (Utilities|FlowControl|Sequence
    (:then_0
      (bind _float_up (Timeline|FloatUp Reverse)
        (:Update
          (for (_array_element _array_index) (Variables|Default|GetFloor)
            (for _array_element_2 (Variables|Default|GetArray1)
              (if (== _array_element_2 _array_element)
                (Transformation|SetWorldLocation _array_element (Math|Vector|Lerp(Vector) (.vector (.Value (Utilities|Map|Find (Variables|Default|GetFallenLoc&Rot) _array_index))) (.vector (.Value (Utilities|Map|Find (Variables|Default|GetDefaultLoc&Rot) _array_index))) _float_up) false false)))))))
    (:then_1
      (bind _roundout (Timeline|RoundOut Reverse)
        (:Update
          (for (_array_element_3 _array_index_2) (Variables|Default|GetFloor)
            (Transformation|SetWorldRotation _array_element_3 (Math|Rotator|Lerp(Rotator) (.rotation (.Value (Utilities|Map|Find (Variables|Default|GetFallenLoc&Rot) _array_index_2))) (.rotation (.Value (Utilities|Map|Find (Variables|Default|GetDefaultLoc&Rot) _array_index_2))) _roundout) false false)))))
    (:then_2
      (bind _delayup (Timeline|DelayUp Reverse)
        (:Update
          (for (_array_element_4 _array_index_3) (Variables|Default|GetFloor)
            (for _array_element_5 (Variables|Default|GetArray2)
              (if (== _array_element_5 _array_element_4)
                (Transformation|SetWorldLocation _array_element_4 (Math|Vector|Lerp(Vector) (.vector (.Value (Utilities|Map|Find (Variables|Default|GetFallenLoc&Rot) _array_index_3))) (.vector (.Value (Utilities|Map|Find (Variables|Default|GetDefaultLoc&Rot) _array_index_3))) _delayup) false false)))))
        (:Finished
          (CallFunction|Finished))))
    (:then_3
      (bind _veryed_float_up (Timeline|VeryFloatUp Reverse)
        (:Update
          (for (_array_element_6 _array_index_4) (Variables|Default|GetFloor)
            (for _array_element_7 (Variables|Default|GetArray3)
              (if (== _array_element_7 _array_element_6)
                (Transformation|SetWorldLocation _array_element_6 (Math|Vector|Lerp(Vector) (.vector (.Value (Utilities|Map|Find (Variables|Default|GetFallenLoc&Rot) _array_index_4))) (.vector (.Value (Utilities|Map|Find (Variables|Default|GetDefaultLoc&Rot) _array_index_4))) _veryed_float_up) false false)))))))))

(event Custom|StayAssembledEnd
  ;[1 1 1] Stay assembled end
  (Variables|Default|SetAllready%20Assembled true)
  (CallFunction|RemoveMovementEffects))

(event Custom|Finished
  ;[1 1 1] Finishe trigered
  (Utilities|FlowControl|Sequence
    (:then_0
      (CallFunction|StopMovementEffects)
      (if (not (Variables|Default|GetMagicBack))
        (CallFunction|Reset)
        (if (Utilities|Time|IsValidTimerHandle (Variables|Default|GetRemoveEffectsTimer)) :!label _label
          (Utilities|Time|ClearandInvalidateTimerbyHandle (Variables|Default|GetRemoveEffectsTimer)))
        (bind _returnvalue (Utilities|Time|SetTimerbyFunctionName 0 "RemoveMovementEffects" 6.0))
        (Variables|Default|SetRemoveEffectsTimer _returnvalue)
        (elif (Variables|Default|GetReveresed)
          (Variables|Default|SetReveresed false)
          (goto _label))))
    (:then_1
      (if (Variables|Default|GetActive)
        (CallFunction|SpecialEventon)))))

(event Custom|SpecialEventOn
  ;[1 1 1] Special events (for lights and stuff)
)

(event Custom|SpecialEventOff
  ;[1 1 1] Special events (for lights and stuff)
)

(event Custom|MovementActivate
  ;[1 1 1] Move the bridge
  (Utilities|FlowControl|Sequence
    (:then_0
      (if (Variables|Default|GetMagicBack)
        (bind _float_up (Timeline|FloatUp Play)
          (:Update
            (for (_array_element _array_index) (Variables|Default|GetFloor)
              (for _array_element_2 (Variables|Default|GetArray1)
                (if (== _array_element_2 _array_element)
                  (Transformation|SetWorldLocation _array_element (Math|Vector|Lerp(Vector) (.vector (.Value (Utilities|Map|Find (Variables|Default|GetFallenLoc&Rot) _array_index))) (.vector (.Value (Utilities|Map|Find (Variables|Default|GetDefaultLoc&Rot) _array_index))) _float_up) false false))))))
        (else
          (Timeline|FloatUp PlayFromStart))))
    (:then_1
      (if (Variables|Default|GetMagicBack)
        (bind _roundout (Timeline|RoundOut Play)
          (:Update
            (for (_array_element_3 _array_index_2) (Variables|Default|GetFloor)
              (Transformation|SetWorldRotation _array_element_3 (Math|Rotator|Lerp(Rotator) (.rotation (.Value (Utilities|Map|Find (Variables|Default|GetFallenLoc&Rot) _array_index_2))) (.rotation (.Value (Utilities|Map|Find (Variables|Default|GetDefaultLoc&Rot) _array_index_2))) _roundout) false false))))
        (else
          (Timeline|RoundOut PlayFromStart))))
    (:then_2
      (if (Variables|Default|GetMagicBack)
        (bind _delayup (Timeline|DelayUp Play)
          (:Update
            (for (_array_element_4 _array_index_3) (Variables|Default|GetFloor)
              (for _array_element_5 (Variables|Default|GetArray2)
                (if (== _array_element_5 _array_element_4)
                  (Transformation|SetWorldLocation _array_element_4 (Math|Vector|Lerp(Vector) (.vector (.Value (Utilities|Map|Find (Variables|Default|GetFallenLoc&Rot) _array_index_3))) (.vector (.Value (Utilities|Map|Find (Variables|Default|GetDefaultLoc&Rot) _array_index_3))) _delayup) false false)))))
          (:Finished
            (CallFunction|Finished)))
        (else
          (Timeline|DelayUp PlayFromStart))))
    (:then_3
      (if (Variables|Default|GetMagicBack)
        (bind _veryed_float_up (Timeline|VeryFloatUp Play)
          (:Update
            (for (_array_element_6 _array_index_4) (Variables|Default|GetFloor)
              (for _array_element_7 (Variables|Default|GetArray3)
                (if (== _array_element_7 _array_element_6)
                  (Transformation|SetWorldLocation _array_element_6 (Math|Vector|Lerp(Vector) (.vector (.Value (Utilities|Map|Find (Variables|Default|GetFallenLoc&Rot) _array_index_4))) (.vector (.Value (Utilities|Map|Find (Variables|Default|GetDefaultLoc&Rot) _array_index_4))) _veryed_float_up) false false))))))
        (else
          (Timeline|VeryFloatUp PlayFromStart))))))

(event EventBeginPlay
  ;[1 1 1] Things Set on spawn
  (CallFunction|SetArray)
  (CallFunction|SetProblematicArray)
  (CallFunction|SetAssembleSpeed)
  (CallFunction|SpecialEventOff)
  (if (not (Variables|Default|GetSpecialActiveAtStart))
    (if (not (Variables|Default|GetUseCustomStartLoc))
      (if (Variables|Default|GetSimAtStart) :!label _label
        (for (_array_element _array_index) (Variables|Default|GetFloor)
          (Utilities|Map|Add (Variables|Default|GetDefaultLoc&Rot) _array_index (Utilities|Struct|MakeS_VectorAndRotation (.location (Transformation|GetWorldTransform _array_element)) (.rotation (Transformation|GetWorldTransform _array_element))))
          (Physics|SetSimulatePhysics _array_element true))
        (Utilities|FlowControl|Sequence
          (:then_0
            (Utilities|PeacefulDisassembly 2.0))
          (:then_1
            (Utilities|FlowControl|Delay 1e+01)
            (CallFunction|EndSim)
            (for (_array_element_2 _array_index_2) (Variables|Default|GetFloor)
              (Utilities|Map|Add (Variables|Default|GetFallenLoc&Rot) _array_index_2 (Utilities|Struct|MakeS_VectorAndRotation (.location (Transformation|GetWorldTransform _array_element_2)) (.rotation (Transformation|GetWorldTransform _array_element_2))))))))
      (elif (not (Class|KismetMathLibrary|EqualExactlyVectorVector (.vector (.Value (Utilities|Map|Find (Variables|Default|GetFallenLoc&Rot) 0))) "0, 0, 0"))
        (for (_array_element_3 _array_index_3) (Variables|Default|GetFloor)
          (Utilities|Map|Add (Variables|Default|GetDefaultLoc&Rot) _array_index_3 (Utilities|Struct|MakeS_VectorAndRotation (.location (Transformation|GetWorldTransform _array_element_3)) (.rotation (Transformation|GetWorldTransform _array_element_3))))
          (Transformation|SetWorldLocationAndRotation _array_element_3 (.vector (.Value (Utilities|Map|Find (Variables|Default|GetFallenLoc&Rot) _array_index_3))) (.rotation (.Value (Utilities|Map|Find (Variables|Default|GetFallenLoc&Rot) _array_index_3))) false true))
        (else
          (goto _label))))
    (else
      (CallFunction|SpecialEventon))))

(event Collision|EventHit
  (params (MyComp :type Primitive%20Component%20Object%20Reference) (Other :type Actor%20Object%20Reference) (OtherComp :type Primitive%20Component%20Object%20Reference) (bSelfMoved :type Boolean) (HitLocation :type Vector :default "0, 0, 0") (HitNormal :type Vector :default "0, 0, 0") (NormalImpulse :type Vector :default "0, 0, 0") (Hit :type Hit%20Result%20Structure%20%28by%20ref%29))
  ;[1 1 1] Hit effect(Plays Sounds and particles when falls apart)
  (CallFunction|HitEffect MyComp NormalImpulse Hit :!label _label)
  (Utilities|FlowControl|Delay 0.2)
  (Utilities|FlowControl|DoOnce false ; enters at Reset
    (:Completed
      (goto _label))))

(fn ConstructionScript)

(fn SoundsSelect
  (params (Component :type Scene%20Component%20Object%20Reference) (Index :type Integer) (Normal%20Impulse :type Vector))
  (bind _volume (Variables|Default|GetVolume))
  (bind _returnvalue (* 7e+05 _volume))
  (bind _returnvalue_2 (- 1e+06 _returnvalue))
  (Audio|SpawnSoundatLocation (Utilities|Array|Get(acopy) (Variables|Default|GetSoundSelect) (select (< Index (Utilities|Array|Length (Variables|Default|GetSoundSelect))) Index 0)) (Transformation|GetWorldLocation Component) "0, 0, 0" (select (Variables|Default|GetSilent) 0.0 (/ (Math|Vector|VectorLength Normal%20Impulse) (Math|Float|Clamp(Float) _returnvalue_2 1e+02 _returnvalue_2))) 1.0 0.0 "/Game/DATA/SoundFX/MasterSoundFiles/SA_Smallobjects.SA_Smallobjects" 0))

(fn SpawnEffect
  (params (Hit%20Info :type Hit%20Result%20Structure) (SystemTemplate :type Niagara%20System%20Object%20Reference) (Normal%20Impulse :type Vector))
  (bind (_bblockinghit _binitialoverlap _time _distance _location _impactpoint _normal) (Collision|BreakHitResult Hit%20Info))
  (bind _particlesize (Variables|Default|GetParticleSize))
  (bind _returnvalue (* 1e+05 _particlesize))
  (bind _returnvalue_2 (- 2e+05 _returnvalue))
  (Niagara|SpawnSystematLocation SystemTemplate _location (Math|Conversions|RotationFromXVector _normal) (Math|Conversions|ToVector(Float) (/ (Math|Vector|VectorLength Normal%20Impulse) (Math|Float|Clamp(Float) _returnvalue_2 1e+02 _returnvalue_2)))))

(fn HitEffect
  (params (Component :type Scene%20Component%20Object%20Reference) (Normal%20Impulse :type Vector) (HitInfo :type Hit%20Result%20Structure))
  (if (> (/ (Math|Vector|VectorLength Normal%20Impulse) 1e+05) 0.4)
    (switch Utilities|FlowControl|Switch|SwitchonEPhysicalSurface (Variables|/Script/PhysicsCore.PhysicalMaterial|GetSurfaceType (.PhysMat (Collision|BreakHitResult HitInfo)))
      (:SurfaceType_Default
        (LocalVariables|SetIndex 0)
        (CallFunction|SpawnEffect HitInfo "/Game/DATA/Particles/Hit/P_Default_Converted.P_Default_Converted" Normal%20Impulse))
      (:SurfaceType1
        (LocalVariables|SetIndex 1)
        (CallFunction|SpawnEffect HitInfo "/Game/DATA/Particles/Hit/P_Default_Converted.P_Default_Converted" Normal%20Impulse))
      (:SurfaceType2
        (LocalVariables|SetIndex 2)
        (CallFunction|SpawnEffect HitInfo "/Game/DATA/Particles/Hit/P_Vegetation_Converted.P_Vegetation_Converted" Normal%20Impulse))
      (:SurfaceType3
        (LocalVariables|SetIndex 3)
        (CallFunction|SpawnEffect HitInfo "/Game/DATA/Particles/Hit/P_Asphalt_Converted.P_Asphalt_Converted" Normal%20Impulse))
      (:SurfaceType4
        (LocalVariables|SetIndex 4)
        (CallFunction|SpawnEffect HitInfo "/Game/DATA/Particles/Hit/P_Dirt.P_Dirt" Normal%20Impulse))
      (:SurfaceType5
        (LocalVariables|SetIndex 5)
        (CallFunction|SpawnEffect HitInfo "/Game/DATA/Particles/Hit/P_Water.P_Water" Normal%20Impulse))
      (:SurfaceType6
        (LocalVariables|SetIndex 6 :!label _label)
        (CallFunction|SpawnEffect HitInfo "/Game/DATA/FX/Particles/Morigesh/Skins/NorthernMystic/P_Morigesh_NorthernMystic_Primary_HitCharacter_Converted.P_Morigesh_NorthernMystic_Primary_HitCharacter_Converted" Normal%20Impulse))
      (:SurfaceType7
        (LocalVariables|SetIndex 7)
        (CallFunction|SpawnEffect HitInfo "/Game/DATA/FX/Particles/Sparrow/Abilities/Primary/FX/P_PROTO_Proto_Ballistic_HitPlayer_Converted.P_PROTO_Proto_Ballistic_HitPlayer_Converted" Normal%20Impulse))
      (:SurfaceType8
        (goto _label))
      (:SurfaceType9
        (LocalVariables|SetIndex 8)
        (CallFunction|SpawnEffect HitInfo "/Game/DATA/Particles/Hit/P_Vegetation_Converted.P_Vegetation_Converted" Normal%20Impulse)))
    (CallFunction|SoundsSelect Component (LocalVariables|GetIndex) Normal%20Impulse)))

(fn SaveInti
  (bind _returnvalue (SaveGame|CreateSaveGameObject "/Game/DATA/Blueprints/SaveGame/BP_BridgeSave.BP_BridgeSave_C"))
  (Variables|Default|SetBridge%20Save _returnvalue))

(fn SaveLoc
  (Variables|Default|SetFallenLoc&Rot (Variables|Default|GetFallenLoc&Rot)))

(fn LoadLoc
  (bind _returnvalue (SaveGame|LoadGamefromSlot (Utilities|GetObjectName self)))
  (bind _asbp_bridge_save (Utilities|Casting|CastToBP_BridgeSave _returnvalue))
  (Variables|Default|SetBridge%20Save _asbp_bridge_save)
  (Variables|Default|SetFallenLoc&Rot (Variables|/Game/DATA/Blueprints/SaveGame/BP_BridgeSave.BP_BridgeSave_C|GetFallenLoc&Rot (Variables|Default|GetBridge%20Save))))

(fn SetAssembleSpeed
  (Components|Timeline|SetPlayRate (Variables|Default|GetFloatUp) (Variables|Default|GetAssembleSpeed))
  (Components|Timeline|SetPlayRate (Variables|Default|GetRoundOut) (Variables|Default|GetAssembleSpeed))
  (Components|Timeline|SetPlayRate (Variables|Default|GetDelayUp) (Variables|Default|GetAssembleSpeed))
  (Components|Timeline|SetPlayRate (Variables|Default|GetVeryFloatUp) (Variables|Default|GetAssembleSpeed)))

(fn SpawnMovementEffects
  (params (MeshIn :type Static%20Mesh%20Component%20Object%20Reference))
  (if (Variables|Default|GetUseMoveSounds)
    (bind _returnvalue (Audio|SpawnSoundAttached "/Game/DATA/SoundFX/MagicSound/SC_MagicStyleOne.SC_MagicStyleOne" MeshIn "None" "0, 0, 0" "0, 0, 0" "KeepRelativeOffset" false 1.0 1.0 0.0 0 0 false))
    (Audio|Components|Audio|SetVolumeMultiplier _returnvalue (Variables|Default|GetMove%20Volume) :!class /Script/Engine.AudioComponent)
    (Utilities|Array|Add (Variables|Default|GetMovmentSound) _returnvalue))
  (if (Variables|Default|GetUseMoveParticles)
    (bind _returnvalue_2 (Niagara|SpawnSystemAttached "/Game/DATA/Particles/P_MagicFlow.P_MagicFlow" MeshIn "None" "0, 0, 0" "0, 0, 0" "KeepRelativeOffset" false))
    (Utilities|Array|Add (Variables|Default|GetMagicFlowPartical) _returnvalue_2)))

(fn StopMovementEffects
  (for _array_element (Variables|Default|GetMovmentSound)
    (Utilities|IsValid _array_element
      (:Is%20Valid
        (Audio|Components|Audio|FadeOut _array_element 2.0 0.0 "Linear" :!class /Script/Engine.AudioComponent))))
  (for _array_element_2 (Variables|Default|GetMagicFlowPartical)
    (Utilities|IsValid _array_element_2
      (:Is%20Valid
        (Components|Activation|Deactivate _array_element_2))))
  (return))

(fn RemoveMovementEffects
  (for _array_element (Variables|Default|GetMovmentSound)
    (Utilities|IsValid _array_element
      (:Is%20Valid
        (Components|DestroyComponent _array_element))))
  (Utilities|Array|Clear (Variables|Default|GetMovmentSound))
  (for _array_element_2 (Variables|Default|GetMagicFlowPartical)
    (Utilities|IsValid _array_element_2
      (:Is%20Valid
        (Components|DestroyComponent _array_element_2))))
  (return))

(fn ReactivateMovementEffects
  (for _array_element (Variables|Default|GetMovmentSound)
    (Utilities|IsValid _array_element
      (:Is%20Valid
        (Audio|Components|Audio|Play _array_element 0.0))))
  (for _array_element_2 (Variables|Default|GetMagicFlowPartical)
    (Utilities|IsValid _array_element_2
      (:Is%20Valid
        (Components|Activation|Activate _array_element_2 true)))))

(fn Reset
  (Utilities|Array|Clear (Variables|Default|GetArray1))
  (Utilities|Array|Clear (Variables|Default|GetArray2))
  (Utilities|Array|Clear (Variables|Default|GetArray3))
  (Variables|Default|SetSet false))