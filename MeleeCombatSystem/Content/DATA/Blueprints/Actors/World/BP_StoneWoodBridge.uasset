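; Stone and wood bridge world actor that groups its static mesh components into named arrays.
; SetArray fills Floor with 27 mesh pieces, and SetProblematicArray fills ProblematicParts with six of those same pieces.
; The file holds no other logic: BeginPlay is disabled, the construction script only calls its parent, and nothing here calls either event or reads the arrays.
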(event EventBeginPlay
  (|CallParentFunction) ; This node is disabled and will not be called.\nDrag off pins to build functionality.
)

(event EventSetArray
  (Variables|Default|SetFloor (Utilities|Array|MakeArray (Variables|Default|GetStaticMesh) (Variables|Default|GetStaticMesh1) (Variables|Default|GetStaticMesh2) (Variables|Default|GetStaticMesh3) (Variables|Default|GetStaticMesh4) (Variables|Default|GetStaticMesh5) (Variables|Default|GetStaticMesh6) (Variables|Default|GetStaticMesh7) (Variables|Default|GetStaticMesh8) (Variables|Default|GetStaticMesh9) (Variables|Default|GetStaticMesh10) (Variables|Default|GetStaticMesh11) (Variables|Default|GetStaticMesh12) (Variables|Default|GetStaticMesh13) (Variables|Default|GetStaticMesh14) (Variables|Default|GetStaticMesh15) (Variables|Default|GetStaticMesh16) (Variables|Default|GetStaticMesh17) (Variables|Default|GetStaticMesh18) (Variables|Default|GetStaticMesh19) (Variables|Default|GetStaticMesh20) (Variables|Default|GetStaticMesh21) (Variables|Default|GetStaticMesh22) (Variables|Default|GetStaticMesh23) (Variables|Default|GetStaticMesh24) (Variables|Default|GetStaticMesh25) (Variables|Default|GetStaticMesh26))))

(event EventSetProblematicArray
  (Variables|Default|SetProblematicParts (Utilities|Array|MakeArray (Variables|Default|GetStaticMesh25) (Variables|Default|GetStaticMesh24) (Variables|Default|GetStaticMesh22) (Variables|Default|GetStaticMesh7) (Variables|Default|GetStaticMesh23) (Variables|Default|GetStaticMesh6))))

(fn ConstructionScript
  (|CallParentFunction))