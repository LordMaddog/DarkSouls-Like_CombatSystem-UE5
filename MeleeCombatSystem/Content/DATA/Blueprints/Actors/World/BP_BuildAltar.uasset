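; World altar actor that lets the player enter build mode.
; Overlapping the activation box shows an "Enter Build Mode" prompt and activates effects; interacting spawns and possesses a BP_BuildPawn near the follow camera and hides hotbars.
; The pawn leaving BuildArea triggers EndBuilding.
; ToCastOrNotToCast caches the player, then passes any actor; Toggle is empty, and resurrect/reset logic is unwired.
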(event OnComponentBeginOverlap(ActivationBox)
  (params (OverlappedComponent :type Primitive%20Component%20Object%20Reference) (OtherActor :type Actor%20Object%20Reference) (OtherComp :type Primitive%20Component%20Object%20Reference) (OtherBodyIndex :type Integer) (bFromSweep :type Boolean) (SweepResult :type Hit%20Result%20Structure%20%28by%20ref%29))
  ;[1 1 1] Overlap with box
  (bind _isplayer (CallFunction|ToCastorNottoCast OtherActor))
  (if _isplayer
    (Rendering|SetVisibility (Variables|Default|GetPickUpText) true false)
    (Components|Activation|Activate (Variables|Default|GetP_Sparks_Converted) true)))

(event OnComponentEndOverlap(ActivationBox)
  (params (OverlappedComponent :type Primitive%20Component%20Object%20Reference) (OtherActor :type Actor%20Object%20Reference) (OtherComp :type Primitive%20Component%20Object%20Reference) (OtherBodyIndex :type Integer))
  ;[1 1 1] Overlap with box
  (bind _isplayer (CallFunction|ToCastorNottoCast OtherActor))
  (if _isplayer
    (Rendering|SetVisibility (Variables|Default|GetPickUpText) false false)
    (Components|Activation|Deactivate (Variables|Default|GetP_Sparks_Converted))
    (if (Variables|/Game/DATA/Blueprints/Components/StatsComponent.StatsComponent_C|GetUIActive? (Variables|/Game/DATA/BP_PC.BP_PC_C|GetStatsComponent (Variables|Default|GetPlayer)))
      (CallFunction|Toggle))))

(event OnComponentEndOverlap(BuildArea)
  (params (OverlappedComponent :type Primitive%20Component%20Object%20Reference) (OtherActor :type Actor%20Object%20Reference) (OtherComp :type Primitive%20Component%20Object%20Reference) (OtherBodyIndex :type Integer))
  (Variables|Default|GetBuildPawn
    (:then
      (if (== OtherActor (Variables|Default|GetBuildPawn))
        (Default|EndBuilding (Variables|Default|GetBuildPawn))))
    (:else)))

(event Custom|Toggle
  ;[1 1 1] Start Build Mode
)

(event EventBeginPlay
  ;[1 1 1] Set Interact Text
  (bind _ascw_interact_text (Utilities|Casting|CastToCW_InteractText (UserInterface|GetUserWidgetObject (Variables|Default|GetPickUpText))))
  (Rendering|Components|TextRender|SetText (Variables|/Game/DATA/UI/Inventory/CW_InteractText.CW_InteractText_C|GetNameText _ascw_interact_text) "Enter Build Mode")
  (Appearance|SetColorandOpacity (Variables|/Game/DATA/UI/Inventory/CW_InteractText.CW_InteractText_C|GetNameText _ascw_interact_text) (Utilities|Struct|MakeSlateColor "(R=0.166667,G=0.087611,B=0.000000,A=1.000000)") :!class /Script/UMG.TextBlock))

(event EventInteract
  (params (CallEvent :type Actor%20Object%20Reference))
  (bind _player (Variables|Default|GetPlayer))
  (bind _returnvalue (Transformation|GetActorTransform _player))
  ;[1 1 1] Start Build Mode
  (CallFunction|ToCastorNottoCast CallEvent)
  (bind _returnvalue_2 (Game|SpawnActorfromClass "/Game/DATA/BP_BuildPawn.BP_BuildPawn_C" (Math|Transform|MakeTransform (+ (Transformation|GetWorldLocation (Variables|/Game/DATA/BP_PC.BP_PC_C|GetFollowCamera _player)) (* (Transformation|GetActorForwardVector _player) -1e+02)) (.rotation _returnvalue) (.scale _returnvalue)) "Undefined" "MultiplyWithRoot" 0 (Variables|Default|GetPlayer) 0))
  (bind _output_get (Variables|Default|SetBuildPawn _returnvalue_2))
  (Pawn|Possess (Variables|/Game/DATA/BP_PC.BP_PC_C|GetPlayer%20Controller (Variables|Default|GetPlayer)) _output_get)
  (Widget|SetVisibility (Variables|/Game/DATA/UI/Inventory/WBP_MainWidget.WBP_MainWidget_C|GetCW_AbilityHotKeyBar (Variables|/Game/DATA/Blueprints/Actors/Inventory/BP_Inventory.BP_Inventory_C|GetMainWidget (Variables|/Game/DATA/BP_PC.BP_PC_C|GetInventory (Variables|Default|GetPlayer)))) "Collapsed")
  (Rendering|SetVisibility (Variables|Default|GetPickUpText) false false))

(fn ConstructionScript)

(fn ToCastorNottoCast
  (params (InActor :type Actor%20Object%20Reference))
  (bind _player (Variables|Default|GetPlayer)
    (:then
      (if (== (Variables|Default|GetPlayer) _player)
        (return true)))
    (:else
      (bind _asbp_pc (Utilities|Casting|CastToBP_PC InActor)
        (:then
          (if (Variables|/Game/DATA/Blueprints/Components/CombatComponent.CombatComponent_C|GetIsPlayer (Variables|/Game/DATA/BP_PC.BP_PC_C|GetCombatComponent _asbp_pc))
            (Variables|Default|SetPlayer _asbp_pc)
            (return true)))
        (:CastFailed
          (return false))))))