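; BP_Chest is a lootable world chest that shows an "Open Chest" prompt while the player is inside its sphere.
; Overlaps pass through ToCastOrNotToCast, which caches the player-controlled BP_PC and toggles the prompt widget.
; Interact fires once, playing the open animation alongside a timeline-driven rotation.
; After a delay it destroys the sphere and spawns BP_BaseLootDrop at DropLock with the chest's level and loot tables.
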(event OnComponentBeginOverlap(Sphere)
  (params (OverlappedComponent :type Primitive%20Component%20Object%20Reference) (OtherActor :type Actor%20Object%20Reference) (OtherComp :type Primitive%20Component%20Object%20Reference) (OtherBodyIndex :type Integer) (bFromSweep :type Boolean) (SweepResult :type Hit%20Result%20Structure%20%28by%20ref%29))
  (bind _isplayer (CallFunction|ToCastorNottoCast OtherActor))
  (if _isplayer
    (Rendering|SetVisibility (Variables|Default|GetPickUpText) true false)))

(event OnComponentEndOverlap(Sphere)
  (params (OverlappedComponent :type Primitive%20Component%20Object%20Reference) (OtherActor :type Actor%20Object%20Reference) (OtherComp :type Primitive%20Component%20Object%20Reference) (OtherBodyIndex :type Integer))
  (bind _isplayer (CallFunction|ToCastorNottoCast OtherActor))
  (if _isplayer
    (Rendering|SetVisibility (Variables|Default|GetPickUpText) false false)))

(event EventBeginPlay
  (bind _ascw_interact_text (Utilities|Casting|CastToCW_InteractText (UserInterface|GetUserWidgetObject (Variables|Default|GetPickUpText))))
  (Rendering|Components|TextRender|SetText (Variables|/Game/DATA/UI/Inventory/CW_InteractText.CW_InteractText_C|GetNameText _ascw_interact_text) "Open Chest"))

(event Collision|EventActorBeginOverlap
  (params (OtherActor :type Actor%20Object%20Reference)))

(event EventTick
  (params (DeltaSeconds :type Float%20%28single-precision%29)))

(event EventInteract
  (params (CallEvent :type Actor%20Object%20Reference))
  (bind _droplock (Variables|Default|GetDropLock))
  (bind _returnvalue (Transformation|GetWorldLocation _droplock))
  (Utilities|FlowControl|DoOnce false
    (:Completed
      (Components|Animation|PlayAnimation (Variables|Default|GetChest) "/Game/DATA/Meshes/WorldDeco/Chest/Chest_Open.Chest_Open" false)
      (Utilities|FlowControl|Sequence
        (:then_0
          (bind _open (Timeline|Open PlayFromStart)
            (:Update
              (Transformation|SetRelativeRotation (Variables|Default|GetScene) (Math|Rotator|Lerp(Rotator) "0, 0, 0" "0.000000,0.000000,-140.000000" _open) false false))))
        (:then_1
          (Utilities|FlowControl|Delay 1.0)
          (Components|DestroyComponent (Variables|Default|GetSphere))
          (Game|SpawnActorfromClass "/Game/DATA/Blueprints/Actors/BP_BaseLootDrop.BP_BaseLootDrop_C" (Math|Conversions|ToTransform(Vector) _returnvalue) "AlwaysSpawn" "MultiplyWithRoot" self 10 (Variables|Default|GetBoxLEVEL) (Variables|Default|GetLoot%20Table) (Variables|Default|GetLoot%20Table%20Unique) true _returnvalue 0))))))

(fn ConstructionScript)

(fn ToCastorNottoCast
  (params (InActor :type Actor%20Object%20Reference))
  (Utilities|IsValid (Variables|Default|GetPlayer)
    (:Is%20Valid
      (if (== (Variables|Default|GetPlayer) InActor)
        (return true)))
    (:Is%20Not%20Valid
      (bind _asbp_pc (Utilities|Casting|CastToBP_PC InActor)
        (:then
          (if (Variables|/Game/DATA/Blueprints/Components/CombatComponent.CombatComponent_C|GetIsPlayer (Variables|/Game/DATA/BP_PC.BP_PC_C|GetCombatComponent _asbp_pc))
            (Variables|Default|SetPlayer _asbp_pc)
            (return true)))
        (:CastFailed
          (return false))))))