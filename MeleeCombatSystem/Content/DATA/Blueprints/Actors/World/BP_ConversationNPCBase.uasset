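; Base Blueprint for world NPCs the player can interact with to start a conversation.
; BeginPlay hands audio, camera zoom point and mesh to the conversation component, sets up the interact prompt, sends the AnimInstance a look-at-player message and optionally plays a starting montage.
; Box overlaps add or remove it from the interact list via the interact component.
; Interact forwards to that component, then starts the chat with its stored player.
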(event OnComponentBeginOverlap(Box)
  (params (OverlappedComponent :type Primitive%20Component%20Object%20Reference) (OtherActor :type Actor%20Object%20Reference) (OtherComp :type Primitive%20Component%20Object%20Reference) (OtherBodyIndex :type Integer) (bFromSweep :type Boolean) (SweepResult :type Hit%20Result%20Structure%20%28by%20ref%29))
  ;[0.15 0.15 0.15 0.5] Interaction overlap Box
  (bind _isplayer (Default|ToCastorNottoCast (Variables|Default|GetInteractComponent) OtherActor))
  (if _isplayer
    (Default|AddtoInteractList (Variables|Default|GetInteractComponent))))

(event OnComponentEndOverlap(Box)
  (params (OverlappedComponent :type Primitive%20Component%20Object%20Reference) (OtherActor :type Actor%20Object%20Reference) (OtherComp :type Primitive%20Component%20Object%20Reference) (OtherBodyIndex :type Integer))
  ;[0.15 0.15 0.15 0.5] Interaction overlap Box
  (bind _isplayer (Default|ToCastorNottoCast (Variables|Default|GetInteractComponent) OtherActor))
  (if _isplayer
    (Default|RemovefromInteractList (Variables|Default|GetInteractComponent))))

(event EventBeginPlay
  (bind _conversationcomponet (Variables|Default|GetConversationComponet))
  (bind _interactcomponent (Variables|Default|GetInteractComponent))
  (Variables|/Game/DATA/Blueprints/Components/ConversationComponet.ConversationComponet_C|SetAudioComponent _conversationcomponet (Variables|Default|GetAudio))
  (Variables|/Game/DATA/Blueprints/Components/ConversationComponet.ConversationComponet_C|SetCameraZoomLoc _conversationcomponet (Variables|Default|GetCameraZoomLoc))
  (Variables|/Game/DATA/Blueprints/Components/ConversationComponet.ConversationComponet_C|SetMesh _conversationcomponet (Variables|Default|GetSkeletalMesh))
  (Default|Start _interactcomponent self (Variables|Default|GetWidget) (Variables|/Game/DATA/Blueprints/Components/InteractComponent.InteractComponent_C|GetText _interactcomponent) (Variables|/Game/DATA/Blueprints/Components/InteractComponent.InteractComponent_C|GetTextColor _interactcomponent))
  (Class|AnimBPI|LookatTarget(Message) (Components|SkeletalMesh|GetAnimInstance (Variables|Default|GetSkeletalMesh)) (Game|GetPlayerCharacter 0) true)
  (if (Variables|Default|GetUseStarting%20Animation)
    (Animation|Montage|PlayMontage (Variables|Default|GetSkeletalMesh) (Variables|Default|GetStartingAnimation))))

(event EventInteract
  (params (CallEvent :type Actor%20Object%20Reference))
  (bind _interactcomponent (Variables|Default|GetInteractComponent))
  (Default|PInteract _interactcomponent CallEvent)
  (Default|Chat (Variables|Default|GetConversationComponet) (Variables|/Game/DATA/Blueprints/Components/InteractComponent.InteractComponent_C|GetPlayer _interactcomponent)))

(fn ConstructionScript)

(fn GetItemInfo
  (return 0))