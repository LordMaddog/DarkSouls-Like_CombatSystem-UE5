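; Level-up statue where the player spends XP, showing a prompt and particle effects while they are inside its box.
; Interacting toggles the status menu; opening it calls Resurrect on the player, registers the statue with the status screen and resets cutscene and spawn trigger messages.
; Leaving the box closes an open menu.
; ToCastOrNotToCast caches the player, after which its self-comparison passes any actor.
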(event OnComponentBeginOverlap(Box)
  (params (OverlappedComponent :type Primitive%20Component%20Object%20Reference) (OtherActor :type Actor%20Object%20Reference) (OtherComp :type Primitive%20Component%20Object%20Reference) (OtherBodyIndex :type Integer) (bFromSweep :type Boolean) (SweepResult :type Hit%20Result%20Structure%20%28by%20ref%29))
  ;[1 1 1] Overlap with box
  (bind _isplayer (CallFunction|ToCastorNottoCast OtherActor))
  (if _isplayer
    (Rendering|SetVisibility (Variables|Default|GetPickUpText) true false)
    (Components|Activation|Activate (Variables|Default|GetP_Sparks_Converted) true)))

(event OnComponentEndOverlap(Box)
  (params (OverlappedComponent :type Primitive%20Component%20Object%20Reference) (OtherActor :type Actor%20Object%20Reference) (OtherComp :type Primitive%20Component%20Object%20Reference) (OtherBodyIndex :type Integer))
  ;[1 1 1] Overlap with box
  (bind _isplayer (CallFunction|ToCastorNottoCast OtherActor))
  (if _isplayer
    (Rendering|SetVisibility (Variables|Default|GetPickUpText) false false)
    (Components|Activation|Deactivate (Variables|Default|GetP_Sparks_Converted))
    (if (Variables|/Game/DATA/Blueprints/Components/StatsComponent.StatsComponent_C|GetUIActive? (Variables|/Game/DATA/BP_PC.BP_PC_C|GetStatsComponent (Variables|Default|GetPlayer)))
      (CallFunction|Toggle))))

(event Custom|Toggle
  ;[1 1 1] Oppen/Close Status window
  (Class|CombatBPI|ToggleMenu(Message) (Game|GetPlayerController 0))
  (if (Variables|/Game/DATA/Blueprints/Components/StatsComponent.StatsComponent_C|GetUIActive? (Variables|/Game/DATA/BP_PC.BP_PC_C|GetStatsComponent (Variables|Default|GetPlayer)))
    (Utilities|FlowControl|Sequence
      (:then_0
        (Default|Resurrect (Variables|/Game/DATA/BP_PC.BP_PC_C|GetCombatComponent (Variables|Default|GetPlayer)))
        (Components|Activation|Activate (Variables|Default|GetP_Sparks_Converted) true)
        (Rendering|SetVisibility (Variables|Default|GetPickUpText) false false)
        (Variables|/Game/DATA/UI/Menus/StatusScreenUI.StatusScreenUI_C|SetLevelUpStatue (Variables|/Game/DATA/UI/Inventory/WBP_MainWidget.WBP_MainWidget_C|GetStatusScreenUI (Variables|/Game/DATA/Blueprints/Actors/Inventory/BP_Inventory.BP_Inventory_C|GetMainWidget (Variables|/Game/DATA/BP_PC.BP_PC_C|GetInventory (Variables|Default|GetPlayer)))) self))
      (:then_1
        (bind _outactors (Actor|GetAllActorsOfClass "/Game/DATA/Blueprints/Actors/Utility/BP_PlayCutScene.BP_PlayCutScene_C"))
        (for _array_element _outactors
          (Class|CombatBPI|Reset(Message) _array_element)))
      (:then_2
        (bind _outactors_2 (Actor|GetAllActorsOfClass "/Game/DATA/Blueprints/Actors/Utility/BP_SpawnTriger.BP_SpawnTriger_C"))
        (for _array_element_2 _outactors_2
          (Class|SpawnerBPI|ResetSpawn(Message) _array_element_2))))
    (else
      (Components|Activation|Deactivate (Variables|Default|GetP_Sparks_Converted))
      (Rendering|SetVisibility (Variables|Default|GetPickUpText) true false))))

(event EventBeginPlay
  ;[1 1 1] Set Interact Text
  (bind _ascw_interact_text (Utilities|Casting|CastToCW_InteractText (UserInterface|GetUserWidgetObject (Variables|Default|GetPickUpText))))
  (Rendering|Components|TextRender|SetText (Variables|/Game/DATA/UI/Inventory/CW_InteractText.CW_InteractText_C|GetNameText _ascw_interact_text) "Spend XP")
  (Appearance|SetColorandOpacity (Variables|/Game/DATA/UI/Inventory/CW_InteractText.CW_InteractText_C|GetNameText _ascw_interact_text) (Utilities|Struct|MakeSlateColor "(R=0.000000,G=0.338581,B=0.405093,A=1.000000)") :!class /Script/UMG.TextBlock))

(event EventInteract
  (params (CallEvent :type Actor%20Object%20Reference))
  ;[1 1 1] Oppen/Close Status window
  (CallFunction|ToCastorNottoCast CallEvent)
  (Class|CombatBPI|ToggleMenu(Message) (Game|GetPlayerController 0))
  (if (Variables|/Game/DATA/Blueprints/Components/StatsComponent.StatsComponent_C|GetUIActive? (Variables|/Game/DATA/BP_PC.BP_PC_C|GetStatsComponent (Variables|Default|GetPlayer)))
    (Utilities|FlowControl|Sequence
      (:then_0
        (Default|Resurrect (Variables|/Game/DATA/BP_PC.BP_PC_C|GetCombatComponent (Variables|Default|GetPlayer)))
        (Components|Activation|Activate (Variables|Default|GetP_Sparks_Converted) true)
        (Rendering|SetVisibility (Variables|Default|GetPickUpText) false false)
        (Variables|/Game/DATA/UI/Menus/StatusScreenUI.StatusScreenUI_C|SetLevelUpStatue (Variables|/Game/DATA/UI/Inventory/WBP_MainWidget.WBP_MainWidget_C|GetStatusScreenUI (Variables|/Game/DATA/Blueprints/Actors/Inventory/BP_Inventory.BP_Inventory_C|GetMainWidget (Variables|/Game/DATA/BP_PC.BP_PC_C|GetInventory (Variables|Default|GetPlayer)))) self))
      (:then_1
        (bind _outactors (Actor|GetAllActorsOfClass "/Game/DATA/Blueprints/Actors/Utility/BP_PlayCutScene.BP_PlayCutScene_C"))
        (for _array_element _outactors
          (Class|CombatBPI|Reset(Message) _array_element)))
      (:then_2
        (bind _outactors_2 (Actor|GetAllActorsOfClass "/Game/DATA/Blueprints/Actors/Utility/BP_SpawnTriger.BP_SpawnTriger_C"))
        (for _array_element_2 _outactors_2
          (Class|SpawnerBPI|ResetSpawn(Message) _array_element_2))))
    (else
      (Components|Activation|Deactivate (Variables|Default|GetP_Sparks_Converted))
      (Rendering|SetVisibility (Variables|Default|GetPickUpText) true false))))

(fn ConstructionScript)

(fn ToCastorNottoCast
  (params (InActor :type Actor%20Object%20Reference))
  (bind _player (Variables|Default|GetPlayer)
    (:then
      (if (== (Variables|Default|GetPlayer) _player)
        (return true)))
    (:else
      (bind _asbp_pc (Utilities|Casting|CastToBP_PC InActor)
        (:then
          (if (Variables|/Game/DATA/Blueprints/Components/CombatComponent.CombatComponent_C|GetIsPlayer (Variables|/Game/DATA/BP_PC.BP_PC_C|GetCombatComponent _asbp_pc))
            (Variables|Default|SetPlayer _asbp_pc)
            (return true)))
        (:CastFailed
          (return false))))))