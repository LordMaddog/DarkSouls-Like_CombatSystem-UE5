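; Interactable storage chest that the player opens to access a BP_Storage inventory alongside their own.
; Optional starting loot is rolled from DT_ChestStartElement by spawn chance, with generated rarity for some item categories and random stack sizes for others.
; Interact toggles lid animation and storage UI, lazily spawning and reusing one storage actor seeded with that loot.
; A box overlap shows the "Storage" prompt and auto-closes storage when the player leaves.
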(event OnComponentBeginOverlap(Box)
  (params (OverlappedComponent :type Primitive%20Component%20Object%20Reference) (OtherActor :type Actor%20Object%20Reference) (OtherComp :type Primitive%20Component%20Object%20Reference) (OtherBodyIndex :type Integer) (bFromSweep :type Boolean) (SweepResult :type Hit%20Result%20Structure%20%28by%20ref%29))
  ;[1 1 1] Add text over Chest
  (bind _isplayer (CallFunction|ToCastorNottoCast OtherActor))
  (if _isplayer
    (Rendering|SetVisibility (Variables|Default|GetPickUpText) true false)))

(event OnComponentEndOverlap(Box)
  (params (OverlappedComponent :type Primitive%20Component%20Object%20Reference) (OtherActor :type Actor%20Object%20Reference) (OtherComp :type Primitive%20Component%20Object%20Reference) (OtherBodyIndex :type Integer))
  ;[1 1 1] Add text over Chest
  (bind _isplayer (CallFunction|ToCastorNottoCast OtherActor))
  (if _isplayer
    (Rendering|SetVisibility (Variables|Default|GetPickUpText) false false)
    (if (Variables|/Game/DATA/Blueprints/Actors/Inventory/BP_Inventory.BP_Inventory_C|GetStorageOppen (Variables|/Game/DATA/BP_PC.BP_PC_C|GetInventory (Variables|Default|GetPlayer)))
      (CallFunction|OnStorageClose))))

(event Custom|OnStorageClose
  (bind _chest (Variables|Default|GetChest))
  (bind _player (Variables|Default|GetPlayer))
  (bind _inventory (Variables|/Game/DATA/BP_PC.BP_PC_C|GetInventory _player))
  ;[1 1 1] Oppen Close chest
  (Variables|/Script/Engine.SkeletalMeshComponent|SetbPauseAnims (Variables|Default|GetChest) false)
  (Components|Timeline|SetPlayRate _chest -0.9)
  (Audio|Components|Audio|Play _chest false)
  (Variables|/Script/Engine.SkeletalMeshComponent|SetbPauseAnims (Variables|Default|GetChest) false)
  (Utilities|FlowControl|Sequence
    (:then_0
      (bind _open (Timeline|Timeline ReverseFromEnd)
        (:Update
          (Transformation|SetRelativeRotation (Variables|Default|GetScene) (Math|Rotator|Lerp(Rotator) "0, 0, 0" "0.000000,0.000000,-140.000000" _open) false false)
          (Variables|/Script/Engine.SkeletalMeshComponent|SetbPauseAnims (Variables|Default|GetChest) false))
        (:Finished
          (CallFunction|ResetInteract))))
    (:then_1
      (Default|HideStorage (Variables|Default|GetStorageActor))
      (if (Variables|/Game/DATA/Blueprints/Actors/Inventory/BP_Inventory.BP_Inventory_C|GetInventoryVisible (Variables|/Game/DATA/BP_PC.BP_PC_C|GetInventory (Variables|Default|GetPlayer)))
        (Default|HideInventory _inventory)
        (Default|ShowInventory _inventory)
        (Rendering|SetVisibility (Variables|Default|GetPickUpText) true false)))))

(event Custom|ResetInteract
  (bind _player (Variables|Default|GetPlayer))
  (bind _inventory (Variables|/Game/DATA/BP_PC.BP_PC_C|GetInventory _player))
  ;[1 1 1] Oppen Close chest
  (Utilities|FlowControl|DoOnce false) ; enters at Reset
)

(event EventBeginPlay
  ;[1 1 1] Set up Display Text
  (bind _ascw_interact_text (Utilities|Casting|CastToCW_InteractText (UserInterface|GetUserWidgetObject (Variables|Default|GetPickUpText))))
  (Rendering|Components|TextRender|SetText (Variables|/Game/DATA/UI/Inventory/CW_InteractText.CW_InteractText_C|GetNameText _ascw_interact_text) "Storage")
  (Appearance|SetColorandOpacity (Variables|/Game/DATA/UI/Inventory/CW_InteractText.CW_InteractText_C|GetNameText _ascw_interact_text) (Utilities|Struct|MakeSlateColor "(R=0.405093,G=0.211525,B=0.020342,A=1.000000)") :!class /Script/UMG.TextBlock)
  (if (Variables|Default|GetGenerateStartingItems?)
    (CallFunction|GenerateStartingItems)))

(event EventInteract
  (params (CallEvent :type Actor%20Object%20Reference))
  (bind _player (Variables|Default|GetPlayer))
  (bind _inventory (Variables|/Game/DATA/BP_PC.BP_PC_C|GetInventory _player))
  ;[1 1 1] Oppen Close chest
  (Utilities|FlowControl|DoOnce false
    (:Completed
      (bind _isplayer (CallFunction|ToCastorNottoCast CallEvent))
      (if _isplayer
        (if (not (Variables|/Game/DATA/Blueprints/Actors/Inventory/BP_Inventory.BP_Inventory_C|GetStorageOppen (Variables|/Game/DATA/BP_PC.BP_PC_C|GetInventory (Variables|Default|GetPlayer))))
          (Components|Animation|PlayAnimation (Variables|Default|GetChest) "/Game/DATA/Meshes/WorldDeco/Chest/Chest_Open.Chest_Open" false)
          (Rendering|SetVisibility (Variables|Default|GetPickUpText) false false)
          (Utilities|FlowControl|Sequence
            (:then_0
              (bind _open (Timeline|Open PlayFromStart)
                (:Update
                  (Transformation|SetRelativeRotation (Variables|Default|GetScene) (Math|Rotator|Lerp(Rotator) "0, 0, 0" "0.000000,0.000000,-140.000000" _open) false false))
                (:Finished
                  (CallFunction|ResetInteract))))
            (:then_1
              (Utilities|IsValid (Variables|Default|GetStorageActor)
                (:Is%20Valid
                  _)
                (:Is%20Not%20Valid
                  (bind _returnvalue (Game|SpawnActorfromClass "/Game/DATA/Blueprints/Actors/Inventory/BP_Storage.BP_Storage_C" (Math|Transform|MakeTransform "0, 0, 0" "0, 0, 0" "1.000000,1.000000,1.000000") "AlwaysSpawn" "MultiplyWithRoot" 0 (Variables|Default|GetAmountOfSlots) 999 (Variables|Default|GetPlayer) (Variables|Default|GetSlotsPerRow) 5 3.0 false 1e+04 self (Variables|Default|GetStartItems) 0))
                  (Variables|Default|SetStorageActor _returnvalue)))
              (Default|GenerateSlotWidgets (Variables|/Game/DATA/Blueprints/Actors/Inventory/BP_Storage.BP_Storage_C|GetWBP%20Storage (Variables|Default|GetStorageActor)) (Variables|Default|GetStorageActor))
              (Variables|/Game/DATA/Blueprints/Actors/Inventory/BP_Inventory.BP_Inventory_C|SetStorage (Variables|/Game/DATA/BP_PC.BP_PC_C|GetInventory (Variables|Default|GetPlayer)) (Variables|Default|GetStorageActor))
              (Default|ShowStorage (Variables|Default|GetStorageActor))
              (Default|HideInventory _inventory)
              (Default|ShowInventory _inventory)))
          (else
            (CallFunction|OnStorageClose)))))))

(fn ConstructionScript)

(fn ToCastorNottoCast
  (params (InActor :type Actor%20Object%20Reference))
  (Variables|Default|GetPlayer
    (:then
      (if (== (Variables|Default|GetPlayer) InActor)
        _
        (else
          (return false))))
    (:else
      (bind _asbp_pc (Utilities|Casting|CastToBP_PC InActor)
        (:then
          (if (Variables|/Game/DATA/Blueprints/Components/CombatComponent.CombatComponent_C|GetIsPlayer (Variables|/Game/DATA/BP_PC.BP_PC_C|GetCombatComponent _asbp_pc))
            (Variables|Default|SetPlayer _asbp_pc)
            (else
              (return false))))
        (:CastFailed
          (return false)))))
  (return true))

(fn GenerateStartingItems
  (bind _outrownames (DataTable|GetDataTableRowNames "/Game/DATA/Blueprints/DataTables/DT_ChestStartElement.DT_ChestStartElement"))
  (for _array_element _outrownames
    (bind _returnvalue (Utilities|GetDataTableRow "/Game/DATA/Blueprints/DataTables/DT_ChestStartElement.DT_ChestStartElement" _array_element)
      (:then
        (if (and (Utilities|IsValidClass (.itemclass _returnvalue)) (<= (Math|Random|RandomIntegerinRange 1 100) (.spawnchance _returnvalue)))
          (if (Utilities|Enum|Equal(Enum) (.Category (Utilities|Struct|BreakS_ItemInfo (.ItemInfo (Utilities|GetClassDefaults (.itemclass _returnvalue))))) "NewEnumerator0")
            (bind _returnvalue_2 (Game|SpawnActorfromClass (.itemclass _returnvalue) (Math|Transform|MakeTransform "0, 0, 0" "0, 0, 0" "1.000000,1.000000,1.000000") "Undefined" "MultiplyWithRoot" 0 (.ItemInfo (Utilities|GetClassDefaults (.itemclass _returnvalue))) "NewEnumerator0" 1 (.DesiredEquipType (Utilities|GetClassDefaults (.itemclass _returnvalue))) "NewEnumerator0" 0 0 0 "NewEnumerator1" true 0 :!label _label))
            (Default|GenerateRarity _returnvalue_2 0.0)
            (Utilities|Array|Add (Variables|Default|GetStartItems) (Utilities|Struct|MakeS_Inventory (Variables|/Game/DATA/Blueprints/Actors/BP_MasterItem.BP_MasterItem_C|GetItemInfo _returnvalue_2) 1))
            (elif (Utilities|Enum|Equal(Enum) (.Category (Utilities|Struct|BreakS_ItemInfo (.ItemInfo (Utilities|GetClassDefaults (.itemclass _returnvalue))))) "NewEnumerator2")
              (goto _label)
              (else
                (Utilities|Array|Add (Variables|Default|GetStartItems) (Utilities|Struct|MakeS_Inventory (.ItemInfo (Utilities|GetClassDefaults (.itemclass _returnvalue))) (Math|Random|RandomIntegerinRange (.minamount _returnvalue) (.maxamount _returnvalue)))))))))))
  (return))

(fn GetItemInfo
  (return 0))