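; BP_DeathXPDrop is a world pickup, apparently left on death, that lets the player retrieve an XP amount.
; On BeginPlay it fills its interact-text widget with that amount; sphere overlaps show and hide the text for actors passing a cast check.
; Interact fires once, activates a particle effect, then after a short delay adds XP through the player's StatsComponent, plays a sound and destroys the actor.
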(event OnComponentBeginOverlap(Sphere)
  (params (OverlappedComponent :type Primitive%20Component%20Object%20Reference) (OtherActor :type Actor%20Object%20Reference) (OtherComp :type Primitive%20Component%20Object%20Reference) (OtherBodyIndex :type Integer) (bFromSweep :type Boolean) (SweepResult :type Hit%20Result%20Structure%20%28by%20ref%29))
  (bind _isplayer (CallFunction|ToCastorNottoCast OtherActor))
  (if _isplayer
    (Rendering|SetVisibility (Variables|Default|GetPickUpText) true false)))

(event OnComponentEndOverlap(Sphere)
  (params (OverlappedComponent :type Primitive%20Component%20Object%20Reference) (OtherActor :type Actor%20Object%20Reference) (OtherComp :type Primitive%20Component%20Object%20Reference) (OtherBodyIndex :type Integer))
  (bind _isplayer (CallFunction|ToCastorNottoCast OtherActor))
  (if _isplayer
    (Rendering|SetVisibility (Variables|Default|GetPickUpText) false false)))

(event EventBeginPlay
  (bind _ascw_interact_text (Utilities|Casting|CastToCW_InteractText (UserInterface|GetUserWidgetObject (Variables|Default|GetPickUpText))))
  (Rendering|Components|TextRender|SetText (Variables|/Game/DATA/UI/Inventory/CW_InteractText.CW_InteractText_C|GetNameText _ascw_interact_text) (Utilities|Text|FormatText "{Retrive XP} ({Amount})" (Utilities|Text|MakeLiteralText "Retrive XP") (Variables|Default|GetXPGiven)))
  (Appearance|SetColorandOpacity (Variables|/Game/DATA/UI/Inventory/CW_InteractText.CW_InteractText_C|GetNameText _ascw_interact_text) (Utilities|Struct|MakeSlateColor "(R=0.000000,G=0.338581,B=0.405093,A=1.000000)") :!class /Script/UMG.TextBlock))

(event EventInteract
  (params (CallEvent :type Actor%20Object%20Reference))
  (bind _player (Variables|Default|GetPlayer))
  (bind _statscomponent (Variables|/Game/DATA/BP_PC.BP_PC_C|GetStatsComponent _player))
  (Utilities|FlowControl|DoOnce false
    (:Completed
      (Components|Activation|Activate (Variables|Default|GetParticleSystem) true)
      (Utilities|FlowControl|Delay 0.1)
      (Utilities|IsValid _statscomponent
        (:Is%20Valid
          (Default|ModifyXP _statscomponent "NewEnumerator0" (Variables|Default|GetXPGiven))
          (Audio|PlaySoundatLocation "/Game/DATA/SoundFX/XP/SC_Xp.SC_Xp" (Transformation|GetActorLocation) "0, 0, 0" 1.0 1.0 0.0 0 0 0 0)
          (Actor|DestroyActor))))))

(fn ConstructionScript
  (|CallParentFunction))