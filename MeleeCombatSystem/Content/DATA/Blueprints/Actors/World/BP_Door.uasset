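; BP_Door is an interactable double door that swings open with sound and switches linked hallway lights on.
; Interact toggles it through a DoOnce that resets shortly after each swing, driving skeletal animations and timelines that rotate both sides.
; An open door calls Close after ten seconds, turning the lights off.
; Sphere overlap toggles the prompt widget for the cached player; nearby-actor tracking and loot-spawn logic are unconnected.
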(event OnComponentBeginOverlap(Sphere)
  (params (OverlappedComponent :type Primitive%20Component%20Object%20Reference) (OtherActor :type Actor%20Object%20Reference) (OtherComp :type Primitive%20Component%20Object%20Reference) (OtherBodyIndex :type Integer) (bFromSweep :type Boolean) (SweepResult :type Hit%20Result%20Structure%20%28by%20ref%29))
  (bind _isplayer (CallFunction|ToCastorNottoCast OtherActor))
  (if _isplayer
    (Rendering|SetVisibility (Variables|Default|GetPickUpText) true false)))

(event OnComponentEndOverlap(Sphere)
  (params (OverlappedComponent :type Primitive%20Component%20Object%20Reference) (OtherActor :type Actor%20Object%20Reference) (OtherComp :type Primitive%20Component%20Object%20Reference) (OtherBodyIndex :type Integer))
  (bind _isplayer (CallFunction|ToCastorNottoCast OtherActor))
  (if _isplayer
    (Rendering|SetVisibility (Variables|Default|GetPickUpText) false false)))

(event Custom|Reset
  (Utilities|FlowControl|Delay 1.0)
  (Utilities|FlowControl|DoOnce false) ; enters at Reset
)

(event Custom|Close
  (Variables|Default|SetOppen? false)
  (Variables|/Script/Engine.SkeletalMeshComponent|SetbPauseAnims (Variables|Default|GetDoor) false)
  (Components|Animation|PlayAnimation (Variables|Default|GetDoor) "/Game/DATA/Meshes/Door/GateDoor_Anim_Armature_Doors_close.GateDoor_Anim_Armature_Doors_close" false)
  (Utilities|FlowControl|Sequence
    (:then_0
      (bind _open (Timeline|Timeline ReverseFromEnd)
        (:Update
          (Transformation|SetRelativeRotation (Variables|Default|GetScene) (Math|Rotator|Lerp(Rotator) "0, 0, 0" "0.000000,93.500000,0.000000" _open) false false)
          (Transformation|SetRelativeRotation (Variables|Default|GetSceneRight) (Math|Rotator|Lerp(Rotator) "0, 0, 0" "0.000000,-93.500000,0.000000" _open) false false))
        (:Finished
          (CallFunction|Reset)
          (Rendering|Components|TextRender|SetText (Variables|Default|GetText) "Oppen Door"))))
    (:then_1
      (Audio|PlaySoundatLocation "/Game/DATA/SoundFX/Door/SC_DoorClose.SC_DoorClose" (Transformation|GetWorldLocation (Variables|Default|GetDoor)) "0, 0, 0" 1.0 1.0 0.0 0 0 0 0)
      (Utilities|FlowControl|Delay 0.5)
      (Audio|PlaySoundatLocation "/Game/DATA/SoundFX/Door/SC_DoorShut.SC_DoorShut" (Transformation|GetWorldLocation (Variables|Default|GetDoor)) "0, 0, 0" 1.0 1.0 0.0 0 0 0 0)
      (for _array_element (Variables|Default|GetHallwayLight)
        (Default|TurnLightOff _array_element)))))

(event EventBeginPlay
  (bind _ascw_interact_text (Utilities|Casting|CastToCW_InteractText (UserInterface|GetUserWidgetObject (Variables|Default|GetPickUpText))))
  (bind _output_get (Variables|Default|SetText (Variables|/Game/DATA/UI/Inventory/CW_InteractText.CW_InteractText_C|GetNameText _ascw_interact_text)))
  (Rendering|Components|TextRender|SetText _output_get "Open Door"))

(event Collision|EventActorBeginOverlap
  (params (OtherActor :type Actor%20Object%20Reference)))

(event EventTick
  (params (DeltaSeconds :type Float%20%28single-precision%29)))

(event EventInteract
  (params (CallEvent :type Actor%20Object%20Reference))
  (Utilities|FlowControl|DoOnce false
    (:Completed
      (if (not (Variables|Default|GetOppen?))
        (Variables|Default|SetOppen? true)
        (Components|Animation|PlayAnimation (Variables|Default|GetDoor) "/Game/DATA/Meshes/Door/GateDoor_Anim_Armature_Doors_open.GateDoor_Anim_Armature_Doors_open" false)
        (Utilities|FlowControl|Sequence
          (:then_0
            (bind _open (Timeline|Open PlayFromStart)
              (:Update
                (Transformation|SetRelativeRotation (Variables|Default|GetScene) (Math|Rotator|Lerp(Rotator) "0, 0, 0" "0.000000,93.500000,0.000000" _open) false false)
                (Transformation|SetRelativeRotation (Variables|Default|GetSceneRight) (Math|Rotator|Lerp(Rotator) "0, 0, 0" "0.000000,-93.500000,0.000000" _open) false false))
              (:Finished
                (CallFunction|Reset)
                (Rendering|Components|TextRender|SetText (Variables|Default|GetText) "Close Door"))))
          (:then_1
            (Audio|PlaySoundatLocation "/Game/DATA/SoundFX/Door/SC_door-handle.SC_door-handle" (Transformation|GetWorldLocation (Variables|Default|GetDoor)) "0, 0, 0" 1.0 1.0 0.0 0 0 0 0)
            (Utilities|FlowControl|Delay 0.5)
            (Audio|PlaySoundatLocation "/Game/DATA/SoundFX/Door/SC_DoorOpen.SC_DoorOpen" (Transformation|GetWorldLocation (Variables|Default|GetDoor)) "0, 0, 0" 1.0 1.0 0.0 0 0 0 0)
            (for _array_element (Variables|Default|GetHallwayLight)
              (Default|TurnLighton _array_element))
            (Utilities|FlowControl|Delay 1e+01)
            (CallFunction|Close)))
        (else
          (CallFunction|Close))))))

(fn ConstructionScript)

(fn ToCastorNottoCast
  (params (InActor :type Actor%20Object%20Reference))
  (Utilities|IsValid (Variables|Default|GetPlayer)
    (:Is%20Valid
      (if (== (Variables|Default|GetPlayer) InActor)
        (return true)))
    (:Is%20Not%20Valid
      (bind _asbp_pc (Utilities|Casting|CastToBP_PC InActor)
        (:then
          (if (Variables|/Game/DATA/Blueprints/Components/CombatComponent.CombatComponent_C|GetIsPlayer (Variables|/Game/DATA/BP_PC.BP_PC_C|GetCombatComponent _asbp_pc))
            (Variables|Default|SetPlayer _asbp_pc)
            (return true)))
        (:CastFailed
          (return false))))))

(fn GetItemInfo
  (return 0))