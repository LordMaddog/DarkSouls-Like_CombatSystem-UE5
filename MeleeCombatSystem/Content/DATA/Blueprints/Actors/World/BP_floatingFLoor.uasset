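; BP_floatingFLoor is a world floor piece that rises into place as a BP_PC approaches and sinks when it leaves.
; BeginPlay drops the mesh below its placed position and randomizes the trigger box's size from PopUpDistance, varying the pop-up range per instance.
; Box overlap tracks one BP_PC and plays the FloatUp timeline to lerp the mesh up.
; End overlap clears it and reverses a separate timeline to lower the mesh.
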(event OnComponentBeginOverlap(Box)
  (params (OverlappedComponent :type Primitive%20Component%20Object%20Reference) (OtherActor :type Actor%20Object%20Reference) (OtherComp :type Primitive%20Component%20Object%20Reference) (OtherBodyIndex :type Integer) (bFromSweep :type Boolean) (SweepResult :type Hit%20Result%20Structure%20%28by%20ref%29))
  (bind _relative_location (Variables|Default|GetRelative%20Location))
  (Variables|Default|GetCurrent%20PC
    (:then)
    (:else
      (bind _asbp_pc (Utilities|Casting|CastToBP_PC OtherActor))
      (Variables|Default|SetCurrent%20PC _asbp_pc)
      (bind _newtrack_0 (Timeline|FloatUp PlayFromStart)
        (:Update
          (Variables|Default|GetCurrent%20PC
            (:then
              (Transformation|SetRelativeLocation (Variables|Default|GetStaticMesh) (Math|Vector|Lerp(Vector) (- _relative_location "0.000000,0.000000,1000.000000") _relative_location _newtrack_0) false false))
            (:else)))))))

(event OnComponentEndOverlap(Box)
  (params (OverlappedComponent :type Primitive%20Component%20Object%20Reference) (OtherActor :type Actor%20Object%20Reference) (OtherComp :type Primitive%20Component%20Object%20Reference) (OtherBodyIndex :type Integer))
  (bind _relative_location (Variables|Default|GetRelative%20Location))
  (if (== OtherActor (Variables|Default|GetCurrent%20PC))
    (Transformation|SetRelativeLocation (Variables|Default|GetStaticMesh) "0.000000,0.000000,-1000.000000" false false)
    (Variables|Default|SetCurrent%20PC 0)
    (bind _newtrack_0 (Timeline|Timeline ReverseFromEnd)
      (:Update
        (Transformation|SetRelativeLocation (Variables|Default|GetStaticMesh) (Math|Vector|Lerp(Vector) (- _relative_location "0.000000,0.000000,1000.000000") _relative_location _newtrack_0) false false)))))

(event EventBeginPlay
  (bind _popupdistance (Variables|Default|GetPopUpDistance))
  (Variables|Default|SetRelative%20Location (Variables|/Script/Engine.SceneComponent|GetRelativeLocation (Variables|Default|GetStaticMesh)))
  (Transformation|SetRelativeLocation (Variables|Default|GetStaticMesh) (- (Variables|Default|GetRelative%20Location) "0.000000,0.000000,1000.000000") false false)
  (Components|Box|SetBoxExtent (Variables|Default|GetBox) (Math|Conversions|ToVector(Float) (Math|Random|RandomFloatinRange _popupdistance (* _popupdistance 2.5))) true))

(fn ConstructionScript)