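; Base weapon actor for dual wielding, extending its parent weapon with an off-hand mesh that moves between hand and holster sockets as combat toggles.
; Collision activation switches main-hand, off-hand and right-foot hit components, with trail effects and off-hand swing sound.
; Enchantment toggles an off-hand Niagara fire effect sized from sword length.
; WeaponFloat uses timelines to lerp the off-hand weapon to a float socket, add random bobbing, then return it.
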(event OnHit(OffHandWeaponCollosionComponent)
  (params (HitResult :type Hit%20Result%20Structure))
  (CallFunction|ONHIT HitResult))

(event OnHit(RightFoot)
  (params (HitResult :type Hit%20Result%20Structure))
  (CallFunction|ONHIT HitResult))

(event EventBeginPlay
  (|CallParentFunction))

(event Collision|EventActorBeginOverlap
  (params (OtherActor :type Actor%20Object%20Reference))
  (|CallParentFunction OtherActor) ; This node is disabled and will not be called.\nDrag off pins to build functionality.
)

(event EventTick
  (params (DeltaSeconds :type Float%20%28single-precision%29))
  (|CallParentFunction DeltaSeconds) ; This node is disabled and will not be called.\nDrag off pins to build functionality.
)

(event EventEnchantMent
  (params (Active :type Boolean) (Magic%20Type :type E_MagicType%20Enum :default "NewEnumerator0") (StatsEffectPower :type Float%20%28double-precision%29))
  (bind _n_fireenchantmentoh (Variables|Default|GetN_FireEnchantmentOH))
  (|CallParentFunction Active "NewEnumerator0" 0.0)
  (if Active
    (Components|Activation|Activate _n_fireenchantmentoh true)
    (else
      (Components|Activation|Deactivate _n_fireenchantmentoh))))

(event EventWeaponFloat
  (params (FloatAway :type Boolean))
  (bind _offhandweaponmesh (Variables|Default|GetOffHandWeaponMesh))
  (bind _floatmagiceffectoh (Variables|Default|GetFloatMagicEffectOH))
  (|CallParentFunction FloatAway)
  (if FloatAway
    (Components|Activation|Activate _floatmagiceffectoh true)
    (CallFunction|DeActivateDamage)
    (Utilities|FlowControl|DoOnce false :!label _label
      (:Completed
        (Variables|Default|SetStartLock (Transformation|GetWorldLocation (Variables|Default|GetOffHandWeaponMesh)))
        (bind _floattime (Timeline|Timeline_0_0_0 PlayFromStart)
          (:Update
            (bind _returnvalue (Utilities|FloatAwayVectorOH _floattime _floattime FloatAway)))
          (:Finished
            (Utilities|FlowControl|Delay 0.1)
            (Variables|Default|SetRandom%20Float%201 (Math|Random|RandomFloatinRange -1e+01 1e+01) :!label _label_2)
            (Variables|Default|SetRandom%20Float%202 (Math|Random|RandomFloatinRange -1e+01 1e+01))
            (bind _floattime_2 (Timeline|Timeline_2 PlayFromStart)
              (:Update
                (if FloatAway
                  (Transformation|SetWorldLocation (Variables|Default|GetOffHandWeaponMesh) (|Switch_2 _floattime_2 _returnvalue) false false)))
              (:Finished
                (Utilities|FlowControl|RetriggerableDelay 1.0)
                (goto _label_2)))))))
    (else
      (Components|Activation|Deactivate _floatmagiceffectoh)
      (Utilities|FlowControl|Sequence
        (:then_0
          (Variables|Default|SetStartRot (Transformation|GetWorldRotation _offhandweaponmesh))
          (Variables|Default|SetStarLockOH (Transformation|GetWorldLocation _offhandweaponmesh))
          (bind _floattime_3 (Timeline|Timeline_1 PlayFromStart)
            (:Update
              (Utilities|FloatBackVector _floattime_3 _floattime_3 false))
            (:Finished
              (Transformation|AttachComponentToComponent (Variables|Default|GetOffHandWeaponMesh) (Variables|/Script/Engine.Character|GetMesh (Variables|Default|GetEquipped%20Character)) (Variables|Initialization|GetSecond%20weapon%20Hand%20Socket) "SnapToTarget" "SnapToTarget" "SnapToTarget" true))))
        (:then_1
          (goto _label Reset))))))

(event EventBeginEquip
  (|CallParentFunction)
  (Transformation|AttachComponentToComponent (Variables|Default|GetOff-HandEffectLocation) (Variables|Default|GetOffHandWeaponMesh) "WeaponCenter" "SnapToTarget" "SnapToTarget" "SnapToTarget" true)
  (Transformation|AttachComponentToComponent (Variables|Default|GetN_WeaponTrail) (Variables|Default|GetItemStaticMesh) "WeaponCenter" "SnapToTarget" "SnapToTarget" "SnapToTarget" true))

(fn ConstructionScript
  (bind _sword_length (Variables|Default|GetSword%20Length))
  (|CallParentFunction)
  (Effects|Components|ParticleSystem|SetFloatParameter (Variables|Default|GetN_WeaponTrailOH) "Ribbon Width" _sword_length)
  (Effects|Components|ParticleSystem|SetFloatParameter (Variables|Default|GetN_FireEnchantmentOH) "SwordHight" (* _sword_length 2.0))
  (Effects|Components|ParticleSystem|SetFloatParameter (Variables|Default|GetN_FireEnchantmentOH) "SpawnRate" (Variables|Default|GetEnchantmentPower))
  (Effects|Components|ParticleSystem|SetBoolParameter (Variables|Default|GetN_FireEnchantmentOH) "Trail" false))

(fn ActivateCollision
  (params (CollisionPart :type E_CollisionPart%20Enum :default "NewEnumerator0") (MagicLeft :type Boolean))
  (|CallParentFunction CollisionPart MagicLeft)
  (switch Utilities|FlowControl|Switch|SwitchonE_CollisionPart CollisionPart
    (:NewEnumerator0
      (Default|EnableCollision (Variables|Default|GetMainWeaponCollisionComponent))
      (Components|Activation|Activate (Variables|Default|GetN_WeaponTrail) true)
      (Effects|Components|ParticleSystem|SetBoolParameter (Variables|Default|GetEnchantmentEffect) "Trail" true))
    (:NewEnumerator1
      (Default|EnableCollision (Variables|Default|GetOffHandWeaponCollosionComponent))
      (Components|Activation|Activate (Variables|Default|GetN_WeaponTrailOH) true)
      (Effects|Components|ParticleSystem|SetBoolParameter (Variables|Default|GetN_FireEnchantmentOH) "Trail" true)
      (Components|Activation|Activate (Variables|Default|GetSwingSoundOH) true))
    (:NewEnumerator2
      (Default|EnableCollision (Variables|Default|GetRightFoot)))))

(fn DeactivateCollision
  (params (CollisionPart :type E_CollisionPart%20Enum :default "NewEnumerator0"))
  (|CallParentFunction CollisionPart)
  (switch Utilities|FlowControl|Switch|SwitchonE_CollisionPart CollisionPart
    (:NewEnumerator0
      (Default|DisableCollision (Variables|Default|GetMainWeaponCollisionComponent)))
    (:NewEnumerator1
      (Default|DisableCollision (Variables|Default|GetOffHandWeaponCollosionComponent))
      (Components|Activation|Deactivate (Variables|Default|GetN_WeaponTrailOH))
      (Effects|Components|ParticleSystem|SetBoolParameter (Variables|Default|GetN_FireEnchantmentOH) "Trail" false))
    (:NewEnumerator2
      (Default|DisableCollision (Variables|Default|GetRightFoot)))))

(fn OnEquipped
  (|CallParentFunction)
  (Default|SetCollisionMesh (Variables|Default|GetOffHandWeaponCollosionComponent) (Variables|Default|GetOffHandWeaponMesh))
  (Default|SetCollisionMesh (Variables|Default|GetRightFoot) (Variables|/Script/Engine.Character|GetMesh (Variables|Default|GetEquipped%20Character)))
  (CallFunction|AttachOff-HandWeapon (select (Default|GetCombatEnabled (Variables|Default|GetEquippedCombatComponent)) (Variables|Initialization|GetSecond%20weapon%20Hand%20Socket) (Variables|Initialization|GetSecond%20weapon%20Attach%20Socket)))
  (Default|AddActortoIgnore (Variables|Default|GetMainWeaponCollisionComponent) (Components|GetOwner)))

(fn AttachOff-HandWeapon
  (params (Socket :type Name))
  (Transformation|AttachComponentToComponent (Variables|Default|GetOffHandWeaponMesh) (Variables|/Script/Engine.Character|GetMesh (Variables|Default|GetEquipped%20Character)) Socket "SnapToTarget" "SnapToTarget" "SnapToTarget" true))

(fn ToggleCombat
  (params (CombatEnabled? :type Boolean))
  (|CallParentFunction CombatEnabled?)
  (CallFunction|AttachOff-HandWeapon (select CombatEnabled? (Variables|Initialization|GetSecond%20weapon%20Hand%20Socket) (Variables|Initialization|GetSecond%20weapon%20Attach%20Socket))))