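; BP_MagicStone is a magic stone material actor that builds on a parent class's drop behavior.
; When dropped, it runs the parent logic, sets a fixed rarity, tints the Sparkle effect's initial color to match that rarity and updates its text.
; BeginPlay and construction only call the parent, and a node enabling physics on PlaceMesh is left unconnected.
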(event EventBeginPlay
  (|CallParentFunction))

(event Collision|EventActorBeginOverlap
  (params (OtherActor :type Actor%20Object%20Reference)))

(event EventTick
  (params (DeltaSeconds :type Float%20%28single-precision%29)))

(event EventOnDropped
  (|CallParentFunction)
  (Variables|Default|SetRarity "NewEnumerator7")
  (Effects|Components|ParticleSystem|SetColorParameter (Variables|Default|GetSparkle) "InitialColor" (Utilities|SelectRarityColor (Variables|Default|GetRarity)))
  (CallFunction|UpdateText))

(fn ConstructionScript
  (|CallParentFunction))