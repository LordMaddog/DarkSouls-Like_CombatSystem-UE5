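; Wood shards material drop actor, a child of a parent drop class that supplies the drop and visual logic.
; When dropped, it runs the parent logic, then enlarges its Sphere radius by a compounding ten percent at each of several Amount thresholds.
; The construction script and AddVisualItem only call the parent; leftover logic scattering randomized mesh copies along a spline is disconnected and never runs.
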(event EventBeginPlay
  (|CallParentFunction) ; This node is disabled and will not be called.\nDrag off pins to build functionality.
)

(event Collision|EventActorBeginOverlap
  (params (OtherActor :type Actor%20Object%20Reference)))

(event EventTick
  (params (DeltaSeconds :type Float%20%28single-precision%29)))

(event EventOnDropped
  (bind _sphere (Variables|Default|GetSphere))
  (bind _sphere_2 (Variables|Default|GetSphere))
  (bind _sphere_3 (Variables|Default|GetSphere))
  (bind _sphere_4 (Variables|Default|GetSphere))
  (|CallParentFunction)
  (if (> (Variables|Default|GetAmount) 10)
    (Components|Sphere|SetSphereRadius _sphere_2 (* (Variables|/Script/Engine.SphereComponent|GetSphereRadius _sphere_2) 1.1) true)
    (if (> (Variables|Default|GetAmount) 20)
      (Components|Sphere|SetSphereRadius _sphere_3 (* (Variables|/Script/Engine.SphereComponent|GetSphereRadius _sphere_3) 1.1) true)
      (if (> (Variables|Default|GetAmount) 40)
        (Components|Sphere|SetSphereRadius _sphere_4 (* (Variables|/Script/Engine.SphereComponent|GetSphereRadius _sphere_4) 1.1) true)
        (if (> (Variables|Default|GetAmount) 50)
          (Components|Sphere|SetSphereRadius _sphere (* (Variables|/Script/Engine.SphereComponent|GetSphereRadius _sphere) 1.1) true))))))

(fn ConstructionScript
  (|CallParentFunction))

(fn AddVisualItem
  (|CallParentFunction))