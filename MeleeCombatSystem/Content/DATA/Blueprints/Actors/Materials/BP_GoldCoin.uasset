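; Gold coin item that drops as a physics pickup worth a random amount scaled by the owning loot drop's level.
; Tick or PulltoPlayer impulses the mesh toward the player, with SoulPullSkill deriving range, power and pickup radius from skill stats.
; Sphere overlap credits gold, queues the UI notice, plays effects and destroys the actor.
; Using it from inventory converts the slot's amount into gold.
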(event OnComponentBeginOverlap(Sphere)
  (params (OverlappedComponent :type Primitive%20Component%20Object%20Reference) (OtherActor :type Actor%20Object%20Reference) (OtherComp :type Primitive%20Component%20Object%20Reference) (OtherBodyIndex :type Integer) (bFromSweep :type Boolean) (SweepResult :type Hit%20Result%20Structure%20%28by%20ref%29))
  ;[1 1 1] Pick UP
  (bind _isplayer (CallFunction|ToCastorNottoCast OtherActor))
  (if _isplayer
    (Utilities|FlowControl|DoOnce false
      (:Completed
        (Default|IncreaseGold (Variables|/Game/DATA/BP_PC.BP_PC_C|GetInventory (Variables|Default|GetPlayer)) (Variables|Default|GetAmount))
        (Default|AddItemtoObtaindQueue (Variables|/Game/DATA/Blueprints/Actors/Inventory/BP_Inventory.BP_Inventory_C|GetMainWidget (Variables|/Game/DATA/BP_PC.BP_PC_C|GetInventory (Variables|Default|GetPlayer))) (Variables|Default|GetAmount) (Variables|Default|GetItemInfo))
        (Components|Activation|Activate (Variables|Default|GetSparkle) true)
        (Utilities|FlowControl|Delay 0.2)
        (Actor|DestroyActor)))))

(event EventBeginPlay
  (|CallParentFunction))

(event EventPulltoPlayer
  (params (Actor :type Vector :default "0, 0, 0") (PullPower :type Float%20%28double-precision%29))
  (bind _returnvalue (+ PullPower (Variables|Default|GetPullPower)))
  (bind _returnvalue_2 (Math|Float|Clamp(Float) _returnvalue 0.0 301.0))
  ;[1 1 1] Pull XP
  (Utilities|FlowControl|Sequence
    (:then_0
      (Utilities|IsValid (Variables|Default|GetCharacter)
        (:Is%20Valid
          (if (Physics|IsSimulatingPhysics (Variables|Default|GetDropMesh) "None")
            (Physics|AddImpulse (Variables|Default|GetDropMesh) (+ (* (Math|Vector|GetForwardVector (Math|Rotator|FindLookatRotation (Transformation|GetWorldLocation (Variables|Default|GetDropMesh)) (Transformation|GetActorLocation (Variables|Default|GetCharacter)))) _returnvalue_2) "0.000000,0.000000,8.000000") "None" true)))))
    (:then_1
      (if (> _returnvalue_2 3e+02)
        (Components|Sphere|SetSphereRadius (Variables|Default|GetSphere) 2e+02 true)))))

(event EventTick
  (params (DeltaSeconds :type Float%20%28single-precision%29))
  ;[1 1 1] Pull XP
  (Utilities|IsValid (Variables|Default|GetCharacter)
    (:Is%20Valid
      (if (<= (Math|Vector|Distance(Vector) (Transformation|GetWorldLocation (Variables|Default|GetDropMesh)) (Transformation|GetActorLocation (Variables|Default|GetCharacter))) (Variables|Default|GetDefualtPullDistance))
        (Utilities|FlowControl|Sequence
          (:then_0
            (Utilities|IsValid (Variables|Default|GetCharacter)
              (:Is%20Valid
                (if (Physics|IsSimulatingPhysics (Variables|Default|GetDropMesh) "None")
                  (Physics|AddImpulse (Variables|Default|GetDropMesh) (+ (* (Math|Vector|GetForwardVector (Math|Rotator|FindLookatRotation (Transformation|GetWorldLocation (Variables|Default|GetDropMesh)) (Transformation|GetActorLocation (Variables|Default|GetCharacter)))) (Math|Float|Clamp(Float) (+ (stale EventPulltoPlayer PullPower) (Variables|Default|GetPullPower)) 0.0 301.0)) "0.000000,0.000000,8.000000") "None" true)))))
          (:then_1
            (if (> (Math|Float|Clamp(Float) (+ (stale EventPulltoPlayer PullPower) (Variables|Default|GetPullPower)) 0.0 301.0) 3e+02)
              (Components|Sphere|SetSphereRadius (Variables|Default|GetSphere) 2e+02 true))))))))

(event EventInteract
  (params (CallEvent :type Actor%20Object%20Reference)))

(event EventEventonUsed
  (params (ItemInfo :type S%20Item%20Info%20Structure))
  (bind _index (Variables|Default|GetIndex))
  (bind _inventory (Variables|Default|GetInventory))
  (bind _slots (Variables|/Game/DATA/Blueprints/Actors/Inventory/BP_Inventory.BP_Inventory_C|GetSlots _inventory))
  (bind _amount (Default|GetAmountatIndex _inventory _index _slots))
  ;[1 1 1] Use to gain money
  (Default|IncreaseGold (Variables|/Game/DATA/BP_PC.BP_PC_C|GetInventory (Variables|/Game/DATA/Blueprints/Actors/Inventory/BP_Inventory.BP_Inventory_C|GetPlayer (Variables|Default|GetInventory))) _amount)
  (Default|RemoveItematIndexInventory _inventory _index _amount false _slots))

(event EventOnDropped
  ;[1 1 1] OnSpawned Dropped
  (Utilities|FlowControl|DoOnce false
    (:Completed
      (Collision|IgnoreActorwhenMoving (Variables|Default|GetDropMesh) self true)
      (CallFunction|RemoveEquipMesh)
      (Variables|Default|SetActiveType "NewEnumerator2")
      (bind _asbp_base_loot_drop (Utilities|Casting|CastToBP_BaseLootDrop (Components|GetOwner))
        (:then
          (Variables|Default|SetAmount (* (Variables|/Game/DATA/Blueprints/Actors/BP_BaseLootDrop.BP_BaseLootDrop_C|GetLEVEL _asbp_base_loot_drop) (Math|Random|RandomFloatinRange 1.0 5.0)))
          (CallFunction|ClearDisplayedItems))
        (:CastFailed
          _))
      (CallFunction|AddVisualItem)
      (Utilities|FlowControl|Delay 0.2)
      (CallFunction|UpdateText)
      (Physics|SetSimulatePhysics (Variables|Default|GetDropMesh) true)
      (bind _character (Class|CombatBPI|GetCharacterInfo(Message) (Game|GetPlayerCharacter 0)))
      (Variables|Default|SetCharacter _character))))

(fn ConstructionScript
  (|CallParentFunction))

(fn SoulPullSkill
  (bind _character (Variables|Default|GetCharacter))
  (bind _statscomponent (Variables|/Game/DATA/BP_PC.BP_PC_C|GetStatsComponent _character))
  (bind (_combat_types _mana_cost _stamina_cost _skill_xp _level_up_cost _skill_xpspent _skill_level _available_points _power _effectiveness) (Default|GetSkillStats _statscomponent "(TagName=\"Character.Action.Skill/Magic.SoulPull\")"))
  (bind _returnvalue (- 22 _mana_cost))
  (Variables|Default|SetDefualtPullDistance (* _power 1e+02))
  (Variables|Default|SetPullPower (* _effectiveness 2e+02))
  (Components|Sphere|SetSphereRadius (Variables|Default|GetSphere) (Math|Conversions|ToFloat(Integer) (* (Math|Integer|Clamp(Integer) _returnvalue 2 _returnvalue) 10)) true))