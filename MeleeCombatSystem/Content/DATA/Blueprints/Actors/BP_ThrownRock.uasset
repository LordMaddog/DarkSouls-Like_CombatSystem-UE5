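; BP_ThrownRock is a thrown rock projectile actor that damages what it hits and breaks on impact.
; Its first Hit stops the flight sound, activates impact and explosive sounds plus a rock-break effect, and applies damage to the hit actor.
; After a three-second delay it destroys itself.
; It also supplies a poise damage multiplier as the product of a base multiplier and a further multiplier.
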(event EventBeginPlay
  (|CallParentFunction) ; This node is disabled and will not be called.\nDrag off pins to build functionality.
)

(event Collision|EventActorBeginOverlap
  (params (OtherActor :type Actor%20Object%20Reference)))

(event EventTick
  (params (DeltaSeconds :type Float%20%28single-precision%29))
  (|CallParentFunction DeltaSeconds) ; This node is disabled and will not be called.\nDrag off pins to build functionality.
)

(event EventHit
  (Utilities|FlowControl|DoOnce false
    (:Completed
      (Components|Activation|Deactivate (Variables|Default|GetFlySound))
      (Components|Activation|Activate (Variables|Default|GetImpactSound) false)
      (CallFunction|ApplyDamage (Variables|Default|GetHitActor) (Variables|Default|GetHitInfo))
      (Utilities|FlowControl|Delay 3.0)
      (Actor|DestroyActor))))

(fn ConstructionScript
  (|CallParentFunction))

(fn GetPoiseDamageMutltiplier
  (return (* (Variables|Default|GetBasePoiseDamgeMultiplier) (Variables|Default|GetPoiseDamgeMultiplier))))