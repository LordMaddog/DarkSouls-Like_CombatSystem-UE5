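; BP_MusicArea is a box trigger volume, sized in the construction script, that tells the player's MusicMaster which music area has been entered via a data table row name.
; Begin and end overlap track whether the player is inside, though only entry notifies MusicMaster.
; A helper identifies the player through the combat component's IsPlayer flag and caches it for later comparisons.
; CheckIfPlayerIn rescans current overlaps and returns presence plus the row name.
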(event OnComponentBeginOverlap(Box)
  (params (OverlappedComponent :type Primitive%20Component%20Object%20Reference) (OtherActor :type Actor%20Object%20Reference) (OtherComp :type Primitive%20Component%20Object%20Reference) (OtherBodyIndex :type Integer) (bFromSweep :type Boolean) (SweepResult :type Hit%20Result%20Structure%20%28by%20ref%29))
  (bind _isplayer (CallFunction|ToCastorNottoCast OtherActor))
  (if _isplayer
    (Default|EnterArea (Variables|/Game/DATA/BP_PC.BP_PC_C|GetMusicMaster (Variables|Default|GetPlayer)) (.rowname (Variables|Default|GetDataTable)))
    (Variables|Default|SetPlayerInArea true)))

(event OnComponentEndOverlap(Box)
  (params (OverlappedComponent :type Primitive%20Component%20Object%20Reference) (OtherActor :type Actor%20Object%20Reference) (OtherComp :type Primitive%20Component%20Object%20Reference) (OtherBodyIndex :type Integer))
  (bind _isplayer (CallFunction|ToCastorNottoCast OtherActor))
  (if _isplayer
    (Variables|Default|SetPlayerInArea false)))

(fn ConstructionScript
  (Components|Box|SetBoxExtent (Variables|Default|GetBox) (Variables|Default|GetIn%20Box%20Extent) true))

(fn ToCastorNottoCast
  (params (InActor :type Actor%20Object%20Reference))
  (Utilities|IsValid (Variables|Default|GetPlayer)
    (:Is%20Valid
      (if (== (Variables|Default|GetPlayer) InActor)
        _
        (else
          (return false))))
    (:Is%20Not%20Valid
      (bind _character (Class|CombatBPI|GetCharacterInfo(Message) InActor))
      (Utilities|IsValid _character
        (:Is%20Valid
          (if (Variables|/Game/DATA/Blueprints/Components/CombatComponent.CombatComponent_C|GetIsPlayer (Variables|/Game/DATA/BP_PC.BP_PC_C|GetCombatComponent _character))
            (Variables|Default|SetPlayer _character)
            (else
              (return false))))
        (:Is%20Not%20Valid
          (return false)))))
  (return true))

(fn CheckifPlayerin
  (for _array_element (Collision|GetOverlappingActors (Variables|Default|GetBox) 0 :!class /Script/Engine.PrimitiveComponent)
    (bind _isplayer (CallFunction|ToCastorNottoCast _array_element))
    (if _isplayer
      (bind _output_get (Variables|Default|SetPlayerInArea true))
      (return _output_get (.rowname (Variables|Default|GetDataTable)))))
  (bind _output_get_2 (Variables|Default|SetPlayerInArea false))
  (return _output_get_2 (.rowname (Variables|Default|GetDataTable))))