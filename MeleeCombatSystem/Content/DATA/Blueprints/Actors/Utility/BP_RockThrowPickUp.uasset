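; Interactable pickup that unlocks the Rock Throw ability for the player, with floating text labelled from its Stat enum.
; On interact it calls Empowered on the player's combat component, then adds its item to the ability slots and the used-ability slots.
; A successful add enables double jump if flagged, replaces on-screen message widgets with a hardcoded unlock message and destroys the pickup.
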(event EventBeginPlay
  (bind _ascw_interact_text (Utilities|Casting|CastToCW_InteractText (UserInterface|GetUserWidgetObject (Variables|Default|GetPickUpText))))
  (Rendering|Components|TextRender|SetText (Variables|/Game/DATA/UI/Inventory/CW_InteractText.CW_InteractText_C|GetNameText _ascw_interact_text) (Utilities|Text|FormatText "{Description} {Power}" (Utilities|Text|MakeLiteralText "New Power") (Utilities|String|EnumtoString (Variables|Default|GetStat)))))

(event EventInteract
  (params (CallEvent :type Actor%20Object%20Reference))
  (bind _asbp_pc (Utilities|Casting|CastToBP_PC CallEvent))
  (Default|Empowered (Variables|/Game/DATA/BP_PC.BP_PC_C|GetCombatComponent _asbp_pc))
  (bind _success_ (Default|AddItemAlt (Variables|/Game/DATA/BP_PC.BP_PC_C|GetInventory _asbp_pc) (.SelfReff (Utilities|Struct|BreakS_ItemInfo (Variables|Default|GetItemInfo))) 1 false (Variables|/Game/DATA/Blueprints/Actors/Inventory/BP_Inventory.BP_Inventory_C|GetSlotsAbilitys (Variables|/Game/DATA/BP_PC.BP_PC_C|GetInventory _asbp_pc))))
  (if _success_
    (Default|AddItemAlt (Variables|/Game/DATA/BP_PC.BP_PC_C|GetInventory _asbp_pc) (.SelfReff (Utilities|Struct|BreakS_ItemInfo (Variables|Default|GetItemInfo))) 1 false (Variables|/Game/DATA/Blueprints/Actors/Inventory/BP_Inventory.BP_Inventory_C|GetSlotsAbilitysUsed (Variables|/Game/DATA/BP_PC.BP_PC_C|GetInventory _asbp_pc)))
    (if (Variables|Default|GetIsDoubleJump)
      (Variables|/Script/Engine.Character|SetJumpMaxCount _asbp_pc 2))
    (bind _foundwidgets (Widget|GetAllWidgetsOfClass "/Game/DATA/UI/BP_MessageWidget.BP_MessageWidget_C" false))
    (for _array_element _foundwidgets
      (Widget|RemovefromParent _array_element))
    (bind _returnvalue (UserInterface|CreateWidget "/Game/DATA/UI/BP_MessageWidget.BP_MessageWidget_C" (Game|GetPlayerController 0) "ROCK THROW UNLOCKED"))
    (UserInterface|Viewport|AddtoViewport _returnvalue 0)
    (Utilities|FlowControl|Sequence
      (:then_0
        (Actor|DestroyActor)))))

(fn ConstructionScript
  (|CallParentFunction))