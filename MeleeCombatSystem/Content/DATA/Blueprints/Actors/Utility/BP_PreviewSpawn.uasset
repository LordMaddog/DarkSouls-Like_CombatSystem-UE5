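; BP_PreviewSpawn is a placement preview actor that shows a group of mesh copies, tinted green or red for whether they are placeable.
; Spawn spreads NumberCount points around Preview in a golden-angle spiral, then attaches collision-free copies of its mesh at all but the first point.
; ChangeColor swaps every material slot on Preview and its copies.
; Nothing in this Blueprint calls Spawn on a live path.
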(event EventBeginPlay)

(fn ConstructionScript)

(fn ChangeColor
  (params (IsPlaceable :type Boolean))
  (for _array_element (Variables|Default|GetPreviews)
    (for _index (range 0 (- (Rendering|Material|GetNumMaterials _array_element) 1))
      (if IsPlaceable
        (Rendering|Material|SetMaterial _array_element _index "/Game/DATA/Meshes/BuildingItems/GreenColor.GreenColor")
        (else
          (Rendering|Material|SetMaterial _array_element _index "/Game/DATA/Meshes/BuildingItems/RedColor.RedColor"))))))

(fn Spawn
  (LocalVariables|SetL_Center (Transformation|GetWorldLocation (Variables|Default|GetPreview)))
  (for _index (range 0 (- (Variables|Default|GetNumberCount) 1))
    (LocalVariables|SetL_Angle (* (Math|Conversions|ToFloat(Integer) (+ _index (Variables|Default|GetAddedAngle))) 2.39996))
    (LocalVariables|SetL_Radius (* (+ (Math|Conversions|ToFloat(Integer) _index) 5.0) (Variables|Default|GetSpaceing)))
    (LocalVariables|SetL_CosAngle (Math|Trig|Cos(Radians) (LocalVariables|GetL_Angle)))
    (LocalVariables|SetL_SinAngle (Math|Trig|Sin(Radians) (LocalVariables|GetL_Angle)))
    (LocalVariables|SetL_X (* (LocalVariables|GetL_CosAngle) (LocalVariables|GetL_Radius)))
    (LocalVariables|SetL_Y (* (LocalVariables|GetL_Radius) (LocalVariables|GetL_SinAngle)))
    (Utilities|Array|Add (Variables|Default|GetLocArray) (Math|Vector|MakeVector (+ (.x (LocalVariables|GetL_Center)) (LocalVariables|GetL_X)) (+ (.y (LocalVariables|GetL_Center)) (LocalVariables|GetL_Y)) (.z (LocalVariables|GetL_Center)))))
  (Utilities|Array|Add (Variables|Default|GetPreviews) (Variables|Default|GetPreview))
  (for (_array_element _array_index) (Variables|Default|GetLocArray)
    (if (> _array_index 0)
      (bind _returnvalue (AddComponent|AddStaticMeshComponent true (Math|Transform|MakeTransform _array_element (Transformation|GetWorldRotation (Variables|Default|GetPreview)) "1.000000,1.000000,1.000000")))
      (Components|StaticMesh|SetStaticMesh _returnvalue (Variables|/Script/Engine.StaticMeshComponent|GetStaticMesh (Variables|Default|GetPreview)))
      (Transformation|AttachComponentToComponent _returnvalue (Variables|Default|GetPreview) "None" "KeepWorld" "KeepWorld" "KeepWorld" true)
      (Collision|SetCollisionEnabled _returnvalue "NoCollision")
      (Utilities|Array|Add (Variables|Default|GetPreviews) _returnvalue))))