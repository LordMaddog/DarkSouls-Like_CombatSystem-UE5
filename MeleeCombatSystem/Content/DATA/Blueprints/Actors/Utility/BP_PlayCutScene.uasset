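; Trigger-box actor that plays a Level Sequence cutscene once when the player character overlaps it.
; BeginPlay creates the sequence player, and a DoOnce gates playback from the box overlap.
; Reset events re-arm that gate and send ResetMessage to every BP_MasterAI.
; Combat and damage functions are stubs, and the teleport-effect binding and delayed stop are disconnected.
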(event OnComponentBeginOverlap(Box)
  (params (OverlappedComponent :type Primitive%20Component%20Object%20Reference) (OtherActor :type Actor%20Object%20Reference) (OtherComp :type Primitive%20Component%20Object%20Reference) (OtherBodyIndex :type Integer) (bFromSweep :type Boolean) (SweepResult :type Hit%20Result%20Structure%20%28by%20ref%29))
  (if (== OtherActor (Game|GetPlayerCharacter 0))
    (Utilities|FlowControl|DoOnce false
      (:Completed
        (Sequencer|Player|Play (Variables|Default|GetSequence) :!class /Script/MovieScene.MovieSceneSequencePlayer)))))

(event OnComponentEndOverlap(Box)
  (params (OverlappedComponent :type Primitive%20Component%20Object%20Reference) (OtherActor :type Actor%20Object%20Reference) (OtherComp :type Primitive%20Component%20Object%20Reference) (OtherBodyIndex :type Integer))
  (if (== OverlappedComponent (Game|GetPlayerCharacter 0))
    (Utilities|FlowControl|DoOnce false
      (:Completed
        (Sequencer|Player|Play (Variables|Default|GetSequence) :!class /Script/MovieScene.MovieSceneSequencePlayer)))))

(event Custom|CallEvent)

(event Custom|Destroy%20and%20Reset
  (CallFunction|ResetOnce)
  (bind _outactors (Actor|GetAllActorsOfClass "/Game/DATA/AI/BP_MasterAI.BP_MasterAI_C"))
  (for _array_element _outactors
    (Utilities|IsValid _array_element
      (:Is%20Valid
        (Class|CombatBPI|Reset(Message) _array_element)))))

(event Custom|ResetOnce
  (Utilities|FlowControl|DoOnce false) ; enters at Reset
)

(event EventBeginPlay
  (bind _returnvalue (Sequencer|Player|CreateLevelSequencePlayer (Variables|Default|GetLevel%20Sequence)))
  (Variables|Default|SetSequence _returnvalue))

(event Collision|EventActorBeginOverlap
  (params (OtherActor :type Actor%20Object%20Reference)))

(event EventTick
  (params (DeltaSeconds :type Float%20%28single-precision%29)))

(event EventReset
  (CallFunction|DestroyandReset))

(fn ConstructionScript)

(fn CanReciveDamage
  (return false))

(fn GetDesiredRotation
  (return "0, 0, 0"))

(fn PreformCombatAction
  (params (ActionTag :type Gameplay%20Tag%20Structure) (SateTag :type Gameplay%20Tag%20Structure) (MontageIndex :type Integer) (bRandomItemIndex :type Boolean))
  (return 0.0))

(fn PreformCombatAttack
  (params (AttackType :type Gameplay%20Tag%20Structure) (SetState :type Gameplay%20Tag%20Structure) (AttackIndex :type Integer) (bRandomIndex :type Boolean))
  (return 0.0))

(fn PreformCustomAction
  (params (ActionTag :type Gameplay%20Tag%20Structure) (StateTag :type Gameplay%20Tag%20Structure) (InMontage :type Anim%20Montage%20Object%20Reference) (MontagePlayRate :type Float%20%28double-precision%29) (bAutoReset :type Boolean))
  (return false))