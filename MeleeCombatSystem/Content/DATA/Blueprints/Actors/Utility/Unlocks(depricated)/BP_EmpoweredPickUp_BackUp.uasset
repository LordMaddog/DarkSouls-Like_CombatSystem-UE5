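; Interactable pickup actor that permanently unlocks a player ability, such as a movement skill or attack, chosen by its Stat variable.
; BeginPlay labels the floating interact text with the power's name.
; Interacting sets the unlock on the player's CombatComponent, triggers Empowered, and raises the jump count when flagged as double jump.
; It then replaces any on-screen message widgets with an unlock announcement and destroys itself.
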(event EventBeginPlay
  (bind _ascw_interact_text (Utilities|Casting|CastToCW_InteractText (UserInterface|GetUserWidgetObject (Variables|Default|GetPickUpText))))
  (Rendering|Components|TextRender|SetText (Variables|/Game/DATA/UI/Inventory/CW_InteractText.CW_InteractText_C|GetNameText _ascw_interact_text) (Utilities|Text|FormatText "{Description} {Power}" (Utilities|Text|MakeLiteralText "New Power") (Utilities|String|EnumtoString (Variables|Default|GetStat)))))

(event EventInteract
  (params (CallEvent :type Actor%20Object%20Reference))
  (bind _asbp_pc (Utilities|Casting|CastToBP_PC CallEvent))
  (Default|SetUnlockState (Variables|/Game/DATA/BP_PC.BP_PC_C|GetCombatComponent _asbp_pc) (Variables|Default|GetStat) true)
  (Default|Empowered (Variables|/Game/DATA/BP_PC.BP_PC_C|GetCombatComponent _asbp_pc))
  (if (Variables|Default|GetIsDoubleJump)
    (Variables|/Script/Engine.Character|SetJumpMaxCount _asbp_pc 2))
  (bind _foundwidgets (Widget|GetAllWidgetsOfClass "/Game/DATA/UI/BP_MessageWidget.BP_MessageWidget_C" false))
  (for _array_element _foundwidgets
    (Widget|RemovefromParent _array_element))
  (bind _returnvalue (UserInterface|CreateWidget "/Game/DATA/UI/BP_MessageWidget.BP_MessageWidget_C" (Game|GetPlayerController 0) (Utilities|Select :Index (Variables|Default|GetStat) :NewEnumerator7 "" :NewEnumerator10 "SPRINTING UNLOCKED" :NewEnumerator8 "CROUCHING UNLOCKED" :NewEnumerator9 "SLIDE UNLOCKED" :NewEnumerator11 "DODGE UNLOCKED" :NewEnumerator1 "DOUBLE JUMP UNLOCKED" :NewEnumerator2 "WALL RUN UNLOCKED" :NewEnumerator5 "MANTLEING UNLOCKED" :NewEnumerator3 "AIR DASH UNLOCKED" :NewEnumerator4 "GRAPPLING HOOK UNLOCKED" :NewEnumerator0 "GLIDE UNLOCKED" :NewEnumerator6 "FLYING UNLOCKED" :NewEnumerator12 "DASH ATTACK UNLOCKED" :NewEnumerator13 "EARTH SMASH UNLOCKED" :NewEnumerator14 "POWER SLASH UNLOCKED" :NewEnumerator15 "ENCHANT WEAPON UNLOCKED" :NewEnumerator16 "WIND PULL UNLOCKED" :NewEnumerator17 "ICE MAGIC UNLOCKED")))
  (UserInterface|Viewport|AddtoViewport _returnvalue 0)
  (Utilities|FlowControl|Sequence
    (:then_0
      (Actor|DestroyActor))))

(fn ConstructionScript
  (|CallParentFunction))