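; Player controller that creates the main HUD and switches the player between gameplay and UI modes.
; BeginPlay caches the primary character, adds the HUD, then after a short delay takes the status menu from the character's inventory.
; Menu and cursor toggles share the UIActive flag, switching input mode, blocking move/look and setting combat state to Attacking while open.
; It also forwards health potion updates to the HUD; combat and damage functions are stubs.
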(event EventBeginPlay
  ;[1 1 1] BeginPlay
  (bind _asbp_pc (Utilities|CasttoPrimaryCharacter 1e+01)
    (:then
      (Variables|Default|SetPlayerC _asbp_pc)
      (Input|SetInputModeGameOnly self false)
      (bind _returnvalue (UserInterface|CreateWidget "/Game/DATA/UI/HUD/BPW_HUD.BPW_HUD_C" self))
      (bind _output_get (Variables|Default|SetMainHud _returnvalue))
      (UserInterface|Viewport|AddtoViewport _output_get 0)
      (Utilities|FlowControl|Delay 1.0)
      (Variables|Default|SetMenu (Variables|/Game/DATA/Blueprints/Actors/Inventory/BP_Inventory.BP_Inventory_C|GetStatus%20Menu (Variables|/Game/DATA/BP_PC.BP_PC_C|GetInventory (Variables|Default|GetPlayerC)))))))

(event EventUpdateHealthPotionAmount
  (params (Amount :type Integer) (Visible? :type Boolean) (ImageStyle :type Slate%20Brush%20Structure))
  (bind _mainhud (Variables|Default|GetMainHud)
    (:then
      (Default|SetPotionAmount _mainhud Amount Visible? ImageStyle))
    (:else)))

(event EventToggleMenu
  ;[1 1 1] Toggle Menu
  (if (not (Variables|/Game/DATA/Blueprints/Components/StatsComponent.StatsComponent_C|GetUIActive? (Variables|/Game/DATA/BP_PC.BP_PC_C|GetStatsComponent (Variables|Default|GetPlayerC))))
    (Variables|/Game/DATA/Blueprints/Components/StatsComponent.StatsComponent_C|SetUIActive? (Variables|/Game/DATA/BP_PC.BP_PC_C|GetStatsComponent (Variables|Default|GetPlayerC)) true)
    (Variables|Default|SetbShowMouseCursor true)
    (Variables|/Script/UMG.Widget|SetVisibility (Variables|Default|GetMenu) "Visible")
    (Default|UpdateStats (Variables|Default|GetMenu))
    (Input|SetIgnoreMoveInput true)
    (Input|SetIgnoreLookInput true)
    (Default|SetState (Variables|/Game/DATA/BP_PC.BP_PC_C|GetCombatComponent (Variables|Default|GetPlayerC)) "(TagName=\"Character.State.Attacking\")")
    (Widget|SetFocus (Variables|/Game/DATA/UI/Menus/StatusScreenUI.StatusScreenUI_C|GetXPEndB (Variables|Default|GetMenu)))
    (Input|SetInputModeGameandUI self (Variables|Default|GetMenu) "DoNotLock" false false)
    (else
      (Variables|/Game/DATA/Blueprints/Components/StatsComponent.StatsComponent_C|SetUIActive? (Variables|/Game/DATA/BP_PC.BP_PC_C|GetStatsComponent (Variables|Default|GetPlayerC)) false)
      (Variables|Default|SetbShowMouseCursor false)
      (Variables|/Script/UMG.Widget|SetVisibility (Variables|Default|GetMenu) "Collapsed")
      (Input|SetIgnoreMoveInput false)
      (Input|SetIgnoreLookInput false)
      (Default|SetState (Variables|/Game/DATA/BP_PC.BP_PC_C|GetCombatComponent (Variables|Default|GetPlayerC)))
      (Input|SetInputModeGameOnly self false))))

(event EventToggleMouseCursor
  ;[1 1 1] Toggle Mouse Cusor
  (if (not (Variables|/Game/DATA/Blueprints/Components/StatsComponent.StatsComponent_C|GetUIActive? (Variables|/Game/DATA/BP_PC.BP_PC_C|GetStatsComponent (Variables|Default|GetPlayerC))))
    (Variables|/Game/DATA/Blueprints/Components/StatsComponent.StatsComponent_C|SetUIActive? (Variables|/Game/DATA/BP_PC.BP_PC_C|GetStatsComponent (Variables|Default|GetPlayerC)) true)
    (Variables|Default|SetbShowMouseCursor true)
    (Input|SetIgnoreMoveInput true)
    (Input|SetIgnoreLookInput true)
    (Default|SetState (Variables|/Game/DATA/BP_PC.BP_PC_C|GetCombatComponent (Variables|Default|GetPlayerC)) "(TagName=\"Character.State.Attacking\")")
    (Input|SetInputModeGameandUI self 0 "DoNotLock" false false)
    (else
      (Variables|/Game/DATA/Blueprints/Components/StatsComponent.StatsComponent_C|SetUIActive? (Variables|/Game/DATA/BP_PC.BP_PC_C|GetStatsComponent (Variables|Default|GetPlayerC)) false)
      (Variables|Default|SetbShowMouseCursor false)
      (Input|ResetIgnoreMoveInput)
      (Input|ResetIgnoreLookInput)
      (Default|SetState (Variables|/Game/DATA/BP_PC.BP_PC_C|GetCombatComponent (Variables|Default|GetPlayerC)))
      (Input|SetInputModeGameOnly self false))))

(fn ConstructionScript)

(fn CanReciveDamage
  (return false))

(fn DamageType
  (return "NewEnumerator0"))

(fn GetDesiredRotation
  (return "0, 0, 0"))

(fn PreformCombatAction
  (params (ActionTag :type Gameplay%20Tag%20Structure) (SateTag :type Gameplay%20Tag%20Structure) (MontageIndex :type Integer) (bRandomItemIndex :type Boolean))
  (return 0.0))

(fn PreformCombatAttack
  (params (AttackType :type Gameplay%20Tag%20Structure) (SetState :type Gameplay%20Tag%20Structure) (AttackIndex :type Integer) (bRandomIndex :type Boolean))
  (return 0.0))

(fn PreformCustomAction
  (params (ActionTag :type Gameplay%20Tag%20Structure) (StateTag :type Gameplay%20Tag%20Structure) (InMontage :type Anim%20Montage%20Object%20Reference) (MontagePlayRate :type Float%20%28double-precision%29) (bAutoReset :type Boolean))
  (return false))