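; Short-lived teleport effect actor that moves the player to the death teleport location and resurrects them.
; On spawn it fetches the destination from BP_DeathTeleportLocation and destroys itself after a delay.
; Player overlap triggers a montage once, resets all BP_PlayCutScene actors, then hides the player and disables movement and collision.
; A timeline lerps them to the destination, where particles and audio play, control is restored and CombatComponent resurrects them.
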(event OnComponentBeginOverlap(Capsule)
  (params (OverlappedComponent :type Primitive%20Component%20Object%20Reference) (OtherActor :type Actor%20Object%20Reference) (OtherComp :type Primitive%20Component%20Object%20Reference) (OtherBodyIndex :type Integer) (bFromSweep :type Boolean) (SweepResult :type Hit%20Result%20Structure%20%28by%20ref%29))
  (if (== OtherActor (Game|GetPlayerCharacter 0))
    (bind _asbp_pc (Utilities|Casting|CastToBP_PC OtherActor))
    (Variables|Default|SetCharacter _asbp_pc)
    (Utilities|FlowControl|DoOnce false
      (:Completed
        (Animation|PlayAnimMontage (Variables|Default|GetCharacter) "/Game/DATA/Animations/Glide/DeathSpawnParticals_Montage.DeathSpawnParticals_Montage" 1.0 "None")
        (Utilities|FlowControl|Sequence
          (:then_0
            (Pawn|Components|CharacterMovement|DisableMovement (Variables|/Script/Engine.Character|GetCharacterMovement (Variables|Default|GetCharacter)))
            (Development|SetHiddeninGame (Variables|/Script/Engine.Character|GetMesh (Variables|Default|GetCharacter)) true true)
            (Utilities|FlowControl|Delay 1.0)
            (Collision|SetActorEnableCollision (Variables|Default|GetCharacter) false)
            (Utilities|IsValid (Variables|Default|GetCharacter)
              (:Is%20Valid
                (Variables|Default|SetStart (Transformation|GetActorLocation (Variables|Default|GetCharacter)))
                (bind _duration (Timeline|TeleportTime PlayFromStart)
                  (:Update
                    (Transformation|SetActorLocation (Variables|Default|GetCharacter) (Math|Vector|Lerp(Vector) (Variables|Default|GetStart) (+ (Variables|Default|GetTeleport%20Lock) "0.000000,0.000000,100.000000") _duration) false true))
                  (:Finished
                    (Transformation|SetActorLocation (- (Transformation|GetWorldLocation (Variables|/Script/Engine.Character|GetMesh (Variables|Default|GetCharacter))) "0,0,15.000000") false true)
                    (Components|Activation|Activate (Variables|Default|GetTeleportParticels) false)
                    (Variables|/Script/Engine.Pawn|SetbUseControllerRotationPitch (Variables|Default|GetCharacter) false)
                    (Transformation|SetActorRotation (Variables|Default|GetCharacter))
                    (Pawn|Components|CharacterMovement|SetMovementMode (Variables|/Script/Engine.Character|GetCharacterMovement (Variables|Default|GetCharacter)) "MOVE_Walking" 0)
                    (Development|SetHiddeninGame (Variables|/Script/Engine.Character|GetMesh (Variables|Default|GetCharacter)) false true)
                    (Collision|SetActorEnableCollision (Variables|Default|GetCharacter) true)
                    (Default|Resurrect (Variables|/Game/DATA/BP_PC.BP_PC_C|GetCombatComponent (Variables|Default|GetCharacter))))))))
          (:then_1
            (bind _outactors (Actor|GetAllActorsOfClass "/Game/DATA/Blueprints/Actors/Utility/BP_PlayCutScene.BP_PlayCutScene_C"))
            (for _array_element _outactors
              (Class|CombatBPI|Reset(Message) _array_element))))))))

(event EventBeginPlay
  (CallFunction|GetTeleLoc)
  (Utilities|FlowControl|Delay 6.0)
  (Actor|DestroyActor))

(fn ConstructionScript)

(fn GetTeleLoc
  (bind _returnvalue (Actor|GetActorOfClass "/Game/DATA/Blueprints/Actors/Utility/BP_DeathTeleportLocation.BP_DeathTeleportLocation_C"))
  (bind _location (Class|GamePlayAbilitiesBPI|GetDeathTeleportLocation(Message) _returnvalue))
  (if (AI|IsValidAILocation _location)
    (Variables|Default|SetTeleport%20Lock _location)))