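; Trigger volume actor that signals linked spawn actors to spawn, on player overlap or optionally at BeginPlay.
; Each signal passes MaxSpawnable to every listed actor, then repeats after a delay while active and respawning is enabled; leaving the box deactivates it.
; Spawned and DoOnce flags gate re-triggering, and ResetSpawn clears the Spawned flag.
; A FlipFlop event toggles custom-depth highlighting on the linked actors' meshes.
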(event OnComponentBeginOverlap(Box)
  (params (OverlappedComponent :type Primitive%20Component%20Object%20Reference) (OtherActor :type Actor%20Object%20Reference) (OtherComp :type Primitive%20Component%20Object%20Reference) (OtherBodyIndex :type Integer) (bFromSweep :type Boolean) (SweepResult :type Hit%20Result%20Structure%20%28by%20ref%29))
  ;[1 1 1] IntSpawn
  (if (== OtherActor (Game|GetPlayerCharacter 0))
    (Variables|Default|SetActive true)
    (if (not (Variables|Default|GetSpawned?))
      (Variables|Default|SetSpawned? true)
      (CallFunction|SendSignaltoSpawn)
      (elif (not (Variables|Options|GetDo%20once?))
        (CallFunction|SendSignaltoSpawn)))))

(event OnComponentEndOverlap(Box)
  (params (OverlappedComponent :type Primitive%20Component%20Object%20Reference) (OtherActor :type Actor%20Object%20Reference) (OtherComp :type Primitive%20Component%20Object%20Reference) (OtherBodyIndex :type Integer))
  ;[1 1 1] SpawnStop
  (if (== OtherActor (Game|GetPlayerCharacter 0))
    (Variables|Default|SetActive false)))

(event Custom|Send%20Signal%20to%20Spawn
  ;[1 1 1] Spawn
  (for _array_element (Variables|Options|GetSpawnActorsToSignal)
    (Class|SpawnerBPI|Spawn(Message) _array_element (Variables|Options|GetMax%20Spawnable)))
  (Utilities|FlowControl|Delay (Variables|Options|GetRespanw%20Delay))
  (if (and (Variables|Default|GetActive) (Variables|Options|GetShouldRespawn?))
    (CallFunction|SendSignaltoSpawn)))

(event Custom|ToggelHilightAtachedActors
  (Utilities|FlowControl|FlipFlop
    (:A
      (for _array_element (Variables|Options|GetSpawnActorsToSignal)
        (bind _mesh (Class|SpawnerBPI|GetMesh(Message) _array_element))
        (Rendering|SetRenderCustomDepth _mesh true)))
    (:B
      (for _array_element_2 (Variables|Options|GetSpawnActorsToSignal)
        (bind _mesh_2 (Class|SpawnerBPI|GetMesh(Message) _array_element_2))
        (Rendering|SetRenderCustomDepth _mesh_2 false)))))

(event EventBeginPlay
  ;[1 1 1] BeginPlay
  (if (Variables|Options|GetSpawnAtStart?)
    ;[1 1 1] IntSpawn
    (Variables|Default|SetActive true)
    (if (not (Variables|Default|GetSpawned?))
      (Variables|Default|SetSpawned? true)
      (CallFunction|SendSignaltoSpawn)
      (elif (not (Variables|Options|GetDo%20once?))
        (CallFunction|SendSignaltoSpawn)))))

(event EventResetSpawn
  (Variables|Default|SetSpawned? false))

(fn ConstructionScript)

(fn GetMesh
  (return 0))