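; World item pickup that simulates physics, can be pulled toward an actor by impulse, and goes into the player's inventory on interaction.
; Construction loads item info from a data table and scatters mesh copies along a spline by Amount, with random rotation and scale.
; Interact records leftovers in LootedPickUps by ID, updating amount and label on partial pickups.
; Live code never destroys the actor; overlap prompt logic is disconnected.
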(event OnComponentBeginOverlap(Sphere)
  (params (OverlappedComponent :type Primitive%20Component%20Object%20Reference) (OtherActor :type Actor%20Object%20Reference) (OtherComp :type Primitive%20Component%20Object%20Reference) (OtherBodyIndex :type Integer) (bFromSweep :type Boolean) (SweepResult :type Hit%20Result%20Structure%20%28by%20ref%29))
  (bind _isplayer (CallFunction|ToCastorNottoCast OtherActor))
  (if (and _isplayer (Variables|Initialize|GetDisplayText?))
    _))

(event OnComponentEndOverlap(Sphere)
  (params (OverlappedComponent :type Primitive%20Component%20Object%20Reference) (OtherActor :type Actor%20Object%20Reference) (OtherComp :type Primitive%20Component%20Object%20Reference) (OtherBodyIndex :type Integer))
  (bind _isplayer (CallFunction|ToCastorNottoCast OtherActor))
  (if (and _isplayer (Variables|Initialize|GetDisplayText?))
    _))

(event OnComponentHit(Cube)
  (params (HitComponent :type Primitive%20Component%20Object%20Reference) (OtherActor :type Actor%20Object%20Reference) (OtherComp :type Primitive%20Component%20Object%20Reference) (NormalImpulse :type Vector :default "0, 0, 0") (Hit :type Hit%20Result%20Structure%20%28by%20ref%29)))

(event Custom|MeshCountDelayCall
  (Utilities|FlowControl|Delay 0.2 :!label _label)
  (bind _continue_ (CallFunction|MeshCount))
  (if _continue_
    (goto _label)))

(event EventPulltoPlayer
  (params (Actor :type Vector :default "0, 0, 0") (PullPower :type Float%20%28double-precision%29))
  (if (and (Variables|Initialize|GetCanBePulled) (Physics|IsSimulatingPhysics (Variables|Default|GetCube) "None"))
    (Physics|AddImpulse (Variables|Default|GetCube) (+ (* (Math|Vector|GetForwardVector (Math|Rotator|FindLookatRotation (Transformation|GetWorldLocation (Variables|Default|GetCube)) Actor)) (Variables|Initialize|GetPullPower)) "0.000000,0.000000,8.000000") "None" true)))

(event EventBeginPlay
  (Collision|IgnoreActorwhenMoving (Variables|Default|GetCube) self true)
  (Utilities|FlowControl|Delay 0.2)
  (Physics|SetSimulatePhysics (Variables|Default|GetCube) true)
  (CallFunction|UpdateText))

(event EventInteract
  (params (CallEvent :type Actor%20Object%20Reference))
  (bind _iteminfo (Variables|Initialize|GetItemInfo))
  (bind _asbp_pc (Utilities|Casting|CastToBP_PC CallEvent))
  (if (Utilities|IsValidClass (.selfreff _iteminfo))
    (bind (_success_ _rest) (Default|AddItemAlt (Variables|/Game/DATA/BP_PC.BP_PC_C|GetInventory _asbp_pc) (Variables|Initialize|GetItemInfo) (.selfreff _iteminfo) (Variables|Initialize|GetAmount) true (Variables|/Game/DATA/Blueprints/Actors/Inventory/BP_Inventory.BP_Inventory_C|GetSlots (Variables|/Game/DATA/BP_PC.BP_PC_C|GetInventory _asbp_pc))))
    (if _success_
      (if (> _rest 0)
        (Variables|Initialize|SetAmount _rest)
        (Utilities|Array|Add (Variables|/Game/DATA/Blueprints/Actors/Inventory/BP_Inventory.BP_Inventory_C|GetLootedPickUps (Variables|/Game/DATA/BP_PC.BP_PC_C|GetInventory _asbp_pc)) (Utilities|Struct|MakeS_SavedPickup (Variables|Initialize|GetID) _rest))
        (CallFunction|UpdateText)
        (Components|Activation|Activate (Variables|Default|GetParticleSystem) false)
        (else
          (Utilities|Array|Add (Variables|/Game/DATA/Blueprints/Actors/Inventory/BP_Inventory.BP_Inventory_C|GetLootedPickUps (Variables|/Game/DATA/BP_PC.BP_PC_C|GetInventory _asbp_pc)) (Utilities|Struct|MakeS_SavedPickup (Variables|Initialize|GetID) 0))
          (Components|Activation|Activate (Variables|Default|GetParticleSystem) false))))
    (else
      (Development|PrintString "false"))))

(fn ConstructionScript
  (CallFunction|UpdateInfo)
  (CallFunction|AddVisualItem))

(fn UpdateText
  (if (Variables|Initialize|GetDisplayText?)
    (bind _ascw_interact_text (Utilities|Casting|CastToCW_InteractText (UserInterface|GetUserWidgetObject (Variables|Default|GetPickUpText)))
      (:then
        (Rendering|Components|TextRender|SetText (Variables|/Game/DATA/UI/Inventory/CW_InteractText.CW_InteractText_C|GetNameText _ascw_interact_text) (Utilities|Text|FormatText "{Name}({amount})" (.itemname (Variables|Initialize|GetItemInfo)) (Variables|Initialize|GetAmount)))
        (return))
      (:CastFailed
        (return)))))

(fn ToCastorNottoCast
  (params (InActor :type Actor%20Object%20Reference))
  (Utilities|IsValid (Variables|Initialize|GetPlayer)
    (:Is%20Valid
      (if (== (Variables|Initialize|GetPlayer) (stale _character))
        _
        (else
          (return false))))
    (:Is%20Not%20Valid
      (bind _character (Class|CombatBPI|GetCharacterInfo(Message) InActor))
      (Utilities|IsValid _character
        (:Is%20Valid
          (if (Variables|/Game/DATA/Blueprints/Components/CombatComponent.CombatComponent_C|GetIsPlayer (Variables|/Game/DATA/BP_PC.BP_PC_C|GetCombatComponent _character))
            (Variables|Initialize|SetPlayer _character)
            (else
              (return false))))
        (:Is%20Not%20Valid
          (return false)))))
  (return true))

(fn MeshCount)

(fn UpdateInfo
  (bind _returnvalue (Utilities|GetDataTableRow "/Game/DATA/Blueprints/DataTables/DepricatedDT_InventoryItemsList.DepricatedDT_InventoryItemsList" (Variables|DataTable|GetItemNameDataTable))
    (:then
      (Variables|Initialize|SetItemInfo _returnvalue))))

(fn AddVisualItem
  (bind _instancesetings (Variables|Default|GetInstanceSetings))
  (bind _cube (Variables|Default|GetCube))
  (bind _cube_2 (Variables|Default|GetCube))
  (bind (_min _max) (Components|StaticMesh|GetLocalBounds _cube_2))
  (bind _output_get (Variables|Default|SetSpacing (+ (.X (Math|Vector|BreakVector (- _max _min))) (Variables|Default|GetSpacingOffset))))
  (bind _output_get_2 (Variables|Default|SetNumberOfInstances (Math|Float|Floor (/ (Spline|GetSplineLength (Variables|Default|GetSpline)) _output_get))))
  (for _index (range 0 _output_get_2)
    (if (>= (- (Variables|Initialize|GetAmount) 1) _index)
      (if (not (== _index 0))
        (bind _returnvalue (AddComponent|AddStaticMeshComponent false (Math|Transform|MakeTransform (Spline|GetLocationatDistanceAlongSpline (Variables|Default|GetSpline) (* (Variables|Default|GetSpacing) _index) "Local") (Math|Rotator|MakeRotator (Math|Random|RandomFloatinRange (.-rx _instancesetings) (.+rx _instancesetings)) (Math|Random|RandomFloatinRange (.-ry _instancesetings) (.+ry _instancesetings)) (Math|Random|RandomFloatinRange (.-rz _instancesetings) (.+rz _instancesetings))) (Math|Vector|MakeVector (Math|Random|RandomFloatinRange (.-sx _instancesetings) (.+sx _instancesetings)) (Math|Random|RandomFloatinRange (.-sy _instancesetings) (.+sy _instancesetings)) (Math|Random|RandomFloatinRange (.-sz _instancesetings) (.+sz _instancesetings))))))
        (Components|StaticMesh|SetStaticMesh _returnvalue (Variables|/Script/Engine.StaticMeshComponent|GetStaticMesh (Variables|Default|GetCube)))
        (Rendering|Material|SetMaterial _returnvalue 0 (Rendering|Material|GetMaterial _cube 0))
        (Transformation|AttachComponentToComponent _returnvalue _cube "None" "KeepWorld" "KeepWorld" "KeepWorld" true)))))

(fn GetItemInfo
  (return 0))