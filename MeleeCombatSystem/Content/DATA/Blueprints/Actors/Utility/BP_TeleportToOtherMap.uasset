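; BP_TeleportToOtherMap is a level-transition trigger that sends the player to another map.
; When the player character overlaps Box, it plays a 2D teleport sound and opens the configured Level reference.
; ShouldBeVisable sets whether the actor shows at BeginPlay.
; A separate VisBox reveals it on any overlap and hides it again when overlap ends, unless it is meant to stay visible.
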(event OnComponentBeginOverlap(Box)
  (params (OverlappedComponent :type Primitive%20Component%20Object%20Reference) (OtherActor :type Actor%20Object%20Reference) (OtherComp :type Primitive%20Component%20Object%20Reference) (OtherBodyIndex :type Integer) (bFromSweep :type Boolean) (SweepResult :type Hit%20Result%20Structure%20%28by%20ref%29))
  (if (== OtherActor (Game|GetPlayerCharacter 0))
    (Audio|PlaySound2D "/Game/DATA/SoundFX/SC_Teleport.SC_Teleport" 1.0 1.0 0.0 0 0)
    (Game|OpenLevel(byObjectReference) (Variables|Default|GetLevel))))

(event OnComponentBeginOverlap(VisBox)
  (params (OverlappedComponent :type Primitive%20Component%20Object%20Reference) (OtherActor :type Actor%20Object%20Reference) (OtherComp :type Primitive%20Component%20Object%20Reference) (OtherBodyIndex :type Integer) (bFromSweep :type Boolean) (SweepResult :type Hit%20Result%20Structure%20%28by%20ref%29))
  (Rendering|SetVisibility (Variables|Default|GetDefaultSceneRoot) true true))

(event OnComponentEndOverlap(VisBox)
  (params (OverlappedComponent :type Primitive%20Component%20Object%20Reference) (OtherActor :type Actor%20Object%20Reference) (OtherComp :type Primitive%20Component%20Object%20Reference) (OtherBodyIndex :type Integer))
  (if (not (Variables|Default|GetShouldBeVisable))
    (Rendering|SetVisibility (Variables|Default|GetDefaultSceneRoot) false true)))

(event EventBeginPlay
  (if (Variables|Default|GetShouldBeVisable)
    (Rendering|SetVisibility (Variables|Default|GetDefaultSceneRoot) true true)
    (else
      (Rendering|SetVisibility (Variables|Default|GetDefaultSceneRoot) false true))))

(event Collision|EventActorBeginOverlap
  (params (OtherActor :type Actor%20Object%20Reference)))

(event EventTick
  (params (DeltaSeconds :type Float%20%28single-precision%29)))

(fn ConstructionScript)