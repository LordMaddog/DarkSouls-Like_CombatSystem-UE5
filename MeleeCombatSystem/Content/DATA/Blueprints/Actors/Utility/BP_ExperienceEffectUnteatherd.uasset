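; Experience particle effect actor that launches in a random direction and homes in on the player's capsule via projectile movement.
; After short startup it activates its Niagara effect, then tightens homing in two delayed stages so it eventually reaches the player.
; Tick applies sprite and ribbon sizes only while a startup flag is set.
; The overlap event is empty; color and sound-then-destroy logic is disconnected.
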(event OnComponentBeginOverlap(SphereCollision)
  (params (OverlappedComponent :type Primitive%20Component%20Object%20Reference) (OtherActor :type Actor%20Object%20Reference) (OtherComp :type Primitive%20Component%20Object%20Reference) (OtherBodyIndex :type Integer) (bFromSweep :type Boolean) (SweepResult :type Hit%20Result%20Structure%20%28by%20ref%29)))

(event EventBeginPlay
  (bind _projectilemovement (Variables|Default|GetProjectileMovement))
  (Utilities|FlowControl|Delay 0.2)
  (Components|Activation|Activate (Variables|Default|GetN_ExperienceParticel) false)
  (Variables|Default|SetDelayFix false)
  (Variables|/Script/Engine.ProjectileMovementComponent|SetHomingTargetComponent (Variables|Default|GetProjectileMovement) (Variables|/Script/Engine.Character|GetCapsuleComponent (Game|GetPlayerCharacter 0)))
  (Utilities|FlowControl|Delay 2.0)
  (Variables|/Script/Engine.ProjectileMovementComponent|SetHomingAccelerationMagnitude _projectilemovement 1e+03)
  (Variables|/Script/Engine.ProjectileMovementComponent|SetMaxSpeed _projectilemovement 7e+02)
  (Utilities|FlowControl|Delay 1e+01)
  (Variables|/Script/Engine.ProjectileMovementComponent|SetHomingAccelerationMagnitude _projectilemovement 1e+05)
  (Variables|/Script/Engine.ProjectileMovementComponent|SetMaxSpeed _projectilemovement 7e+03))

(event EventTick
  (params (DeltaSeconds :type Float%20%28single-precision%29))
  (if (Variables|Default|GetDelayFix)
    (Effects|Components|ParticleSystem|SetFloatParameter (Variables|Default|GetN_ExperienceParticel) "SpriteSize" (Variables|Default|GetSpritSize))
    (Effects|Components|ParticleSystem|SetFloatParameter (Variables|Default|GetN_ExperienceParticel) "RibbonWidth" (Variables|Default|GetRibbonSize))))

(fn ConstructionScript
  (Variables|/Script/Engine.MovementComponent|SetVelocity (Variables|Default|GetProjectileMovement) (Math|Random|RandomUnitVector)))