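; A short-lived utility actor that spawns a decal actor at a hit point and attaches it to what was hit.
; On BeginPlay it orients the spawned Decal class along the impact normal, scaled by either a matched scale or an impact scale.
; Characters get it attached to their mesh at the hit bone, other actors at actor level.
; The helper destroys itself after a brief delay.
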(event EventBeginPlay
  (bind _instigator (Variables|Actor|GetInstigator))
  (bind _hitinfo (Variables|Default|GetHitInfo))
  (bind _hitinfo_2 (Variables|Default|GetHitInfo))
  (bind (_bblockinghit _binitialoverlap _time _distance _location _impactpoint _normal) (Collision|BreakHitResult _hitinfo_2))
  (bind _returnvalue (Game|SpawnActorfromClass (Variables|Default|GetDecal) (Math|Transform|MakeTransform _location (Math|Conversions|RotationFromXVector _normal) (select (Variables|Default|GetScaleMatch?) (Variables|Default|GetMatchedScale) (Math|Conversions|ToVector(Float) (Variables|Default|GetImpactScale)))) "AlwaysSpawn" "MultiplyWithRoot" _instigator _instigator))
  (bind _ascharacter (Utilities|Casting|CastToCharacter (.hitactor _hitinfo))
    (:then
      (Transformation|AttachComponentToComponent _returnvalue (Variables|/Script/Engine.Character|GetMesh _ascharacter) (.hitbonename _hitinfo) "KeepWorld" "KeepWorld" "KeepWorld" true))
    (:CastFailed
      (Transformation|AttachActorToActor _returnvalue (.hitactor _hitinfo) "None" "KeepWorld" "KeepWorld" "KeepWorld" true)))
  (Utilities|FlowControl|Delay 0.2)
  (Actor|DestroyActor))

(fn ConstructionScript)