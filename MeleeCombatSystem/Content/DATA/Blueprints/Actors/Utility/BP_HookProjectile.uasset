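; BP_HookProjectile is a grappling hook projectile that pulls players together or reports a surface hit.
; Hitting a BP_PC deals point damage, attaches the hook, then compares a max stat between owner and target.
; A timeline drags the target in, or pulls the owner over with a montage when the target's stat is higher.
; Other hits notify the owner's CombatComponent, and exceeding max range destroys the hook.
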(event OnComponentHit(Sphere)
  (params (HitComponent :type Primitive%20Component%20Object%20Reference) (OtherActor :type Actor%20Object%20Reference) (OtherComp :type Primitive%20Component%20Object%20Reference) (NormalImpulse :type Vector :default "0, 0, 0") (Hit :type Hit%20Result%20Structure%20%28by%20ref%29))
  (bind _returnvalue (Components|GetOwner))
  (bind _returnvalue_2 (Game|GetInstigator))
  (bind _asbp_pc (Utilities|Casting|CastToBP_PC _returnvalue))
  (Variables|Default|SetHit Hit)
  (Utilities|FlowControl|DoOnce false
    (:Completed
      (bind _asbp_pc_2 (Utilities|Casting|CastToBP_PC OtherActor)
        (:then
          (Variables|Default|SetHitTarget _asbp_pc_2)
          (Game|Damage|ApplyPointDamage OtherActor 1.0 (Transformation|GetActorForwardVector (Components|GetOwner)) (Variables|Default|GetHit) (Pawn|GetController _returnvalue_2) _returnvalue_2 "/Game/DATA/Blueprints/DamageTypes/BP_AttackDamageType.BP_AttackDamageType_C")
          (Collision|SetActorEnableCollision false)
          (Transformation|AttachActorToActor (Variables|Default|GetHitTarget) "None" "KeepWorld" "KeepWorld" "KeepWorld" true)
          (Variables|Default|SetTargetLoc (Transformation|GetActorLocation (Variables|Default|GetHitTarget)))
          (Variables|Default|SetPlayerLoc (Transformation|GetActorLocation (Components|GetOwner)))
          (if (>= (Default|GetMaxStatValue (Variables|/Game/DATA/BP_PC.BP_PC_C|GetStatsComponent _asbp_pc) "NewEnumerator1") (Default|GetMaxStatValue (Variables|/Game/DATA/BP_PC.BP_PC_C|GetStatsComponent (Variables|Default|GetHitTarget)) "NewEnumerator1"))
            (bind _pull (Timeline|Move PlayFromStart)
              (:Update
                (Transformation|SetActorLocation (Variables|Default|GetHitTarget) (Math|Vector|Lerp(Vector) (+ (Variables|Default|GetTargetLoc) "0.000000,0.000000,30.000000") (+ (Variables|Default|GetPlayerLoc) "0.000000,0.000000,30.000000") _pull) true false))
              (:Finished
                (Actor|DestroyActor)))
            (else
              (Animation|PlayAnimMontage _asbp_pc "/Game/DATA/Animations/GrapplingHook/SwingFPulledToEnemy_Montage.SwingFPulledToEnemy_Montage" 1.0 "None")
              (bind _pull_2 (Timeline|Timeline PlayFromStart)
                (:Update
                  (Transformation|SetActorLocation (Components|GetOwner) (Math|Vector|Lerp(Vector) (+ (Variables|Default|GetPlayerLoc) "0.000000,0.000000,30.000000") (+ (Variables|Default|GetTargetLoc) "0.000000,0.000000,30.000000") _pull_2) true false))
                (:Finished
                  (Actor|DestroyActor))))))
        (:CastFailed
          (Class|CombatBPI|GrapplingHookHit(Message) (Actor|GetComponentbyClass (Components|GetOwner) "/Game/DATA/Blueprints/Components/CombatComponent.CombatComponent_C") (.location (Variables|Default|GetHit))))))))

(event EventBeginPlay
  (Collision|IgnoreActorwhenMoving (Variables|Default|GetSphere) (Game|GetInstigator) true)
  (bind _output_get (Variables|Default|SetStaringPostion (Transformation|GetActorLocation))))

(event EventTick
  (params (DeltaSeconds :type Float%20%28single-precision%29))
  (if (> (Math|Vector|Distance(Vector) (stale EventBeginPlay _output_get) (Transformation|GetActorLocation)) (Variables|Default|GetMaxRange))
    (Utilities|FlowControl|DoOnce false
      (:Completed
        (Actor|DestroyActor)))))

(fn ConstructionScript)