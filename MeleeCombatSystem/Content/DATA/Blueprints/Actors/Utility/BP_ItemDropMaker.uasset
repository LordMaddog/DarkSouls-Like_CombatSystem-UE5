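; BP_ItemDropMaker is a utility actor that drops physics-simulated copies of a mesh and saves where they end up.
; On BeginPlay, a delayed loop spawns unattached mesh components at DropLoc until Amount is reached, copying StaticMesh's mesh and first material.
; After a short fixed wait, it stores each component's relative transform in a DroppedItems save object, writes it to a hardcoded slot and prints the result.
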(event EventBeginPlay
  (bind _staticmesh (Variables|Default|GetStaticMesh))
  (Utilities|FlowControl|Delay 0.2)
  (if (< (Variables|Default|GetCurrentAmountSpawned) (Variables|Default|GetAmount)) :!label _label
    (bind _returnvalue (AddComponent|AddStaticMeshComponent true (Math|Transform|MakeTransform (.location (Transformation|GetWorldTransform (Variables|Default|GetDropLoc))) "0, 0, 0" "1.000000,1.000000,1.000000")))
    (Utilities|Array|Add (Variables|Default|GetItems) _returnvalue)
    (Components|StaticMesh|SetStaticMesh _returnvalue (Variables|/Script/Engine.StaticMeshComponent|GetStaticMesh _staticmesh))
    (Physics|SetSimulatePhysics _returnvalue true)
    (Rendering|Material|SetMaterial _returnvalue 0 (Rendering|Material|GetMaterial _staticmesh 0))
    (Utilities|FlowControl|Delay 0.2)
    (Math|Integer|IncrementInt (Variables|Default|GetCurrentAmountSpawned)
      (:%20%20
        (goto _label)))
    (else
      (Utilities|FlowControl|Delay 2.0)
      (for _array_element (Variables|Default|GetItems)
        (Utilities|Array|Add (Variables|Default|GetItemLoc) (Transformation|GetRelativeTransform _array_element)))
      (bind _returnvalue_2 (SaveGame|CreateSaveGameObject "/Game/DATA/Blueprints/SaveGame/DroppedItems.DroppedItems_C"))
      (bind _output_get (Variables|Default|SetSavedData _returnvalue_2))
      (Variables|/Game/DATA/Blueprints/SaveGame/DroppedItems.DroppedItems_C|SetItemLoc _output_get (Variables|Default|GetItemLoc))
      (bind _returnvalue_3 (SaveGame|SaveGametoSlot _output_get "try"))
      (Development|PrintString (Utilities|String|ToString(Boolean) _returnvalue_3)))))

(event Collision|EventActorBeginOverlap
  (params (OtherActor :type Actor%20Object%20Reference)))

(event EventTick
  (params (DeltaSeconds :type Float%20%28single-precision%29)))

(fn ConstructionScript)