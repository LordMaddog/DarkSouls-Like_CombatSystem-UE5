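; Kill-plane volume that damages characters and rescues dropped items that overlap its Cube.
; Characters take point damage equal to a current stat plus a margin, gated by a timed DoOnce shared across all characters.
; Items are teleported to a random navigable point near the player, with physics toggled around the move.
; A MovedItem list, cleared after a delay, prevents repeated moves.
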(event OnComponentBeginOverlap(Cube)
  (params (OverlappedComponent :type Primitive%20Component%20Object%20Reference) (OtherActor :type Actor%20Object%20Reference) (OtherComp :type Primitive%20Component%20Object%20Reference) (OtherBodyIndex :type Integer) (bFromSweep :type Boolean) (SweepResult :type Hit%20Result%20Structure%20%28by%20ref%29))
  (bind _character (Class|CombatBPI|GetCharacterInfo(Message) OtherActor))
  (Utilities|IsValid _character
    (:Is%20Valid
      (Utilities|DoOnce 2.0
        (:then_0
          (Game|Damage|ApplyPointDamage _character (+ (Default|GetCurrentStatValue (Variables|/Game/DATA/BP_PC.BP_PC_C|GetStatsComponent _character) "NewEnumerator1") 1e+01) (.Location (Collision|BreakHitResult SweepResult)) SweepResult 0 self "/Game/DATA/Blueprints/DamageTypes/BP_AttackDamageType.BP_AttackDamageType_C"))))
    (:Is%20Not%20Valid
      (CallFunction|MoveDrop OtherActor)
      (Utilities|FlowControl|Delay 2.0)
      (Utilities|Array|Clear (Variables|Default|GetMovedItem)))))

(event EventBeginPlay)

(event Collision|EventActorBeginOverlap
  (params (OtherActor :type Actor%20Object%20Reference)))

(event EventTick
  (params (DeltaSeconds :type Float%20%28single-precision%29)))

(fn ConstructionScript)

(fn MoveDrop
  (params (Target :type Object%20Object%20Reference))
  (bind _item (Class|InteractableBPI|GetItemInfo(Message) Target))
  (Utilities|IsValid _item
    (:Is%20Valid
      (if (not (Utilities|Array|ContainsItem (Variables|Default|GetMovedItem) _item))
        (Utilities|IsValid (Variables|/Game/DATA/Blueprints/Actors/BP_MasterItem.BP_MasterItem_C|GetDropMesh _item)
          (:Is%20Valid
            (Physics|SetSimulatePhysics (Variables|/Game/DATA/Blueprints/Actors/BP_MasterItem.BP_MasterItem_C|GetDropMesh _item) false)
            (bind _randomlocation (Class|NavigationSystemV1|GetRandomLocationinNavigableRadius (Transformation|GetActorLocation (Game|GetPlayerCharacter 0)) 2e+02 0 0))
            (Utilities|IsValid _item
              (:Is%20Valid
                (Transformation|SetWorldLocation (Variables|/Game/DATA/Blueprints/Actors/BP_MasterItem.BP_MasterItem_C|GetDropMesh _item) (+ _randomlocation "0.000000,0.000000,50.000000") false true)
                (Utilities|IsValid _item
                  (:Is%20Valid
                    (Utilities|Array|Add (Variables|Default|GetMovedItem) _item)
                    (Utilities|IsValid (Variables|/Game/DATA/Blueprints/Actors/BP_MasterItem.BP_MasterItem_C|GetDropMesh _item)
                      (:Is%20Valid
                        (Physics|SetSimulatePhysics (Variables|/Game/DATA/Blueprints/Actors/BP_MasterItem.BP_MasterItem_C|GetDropMesh _item) true)
                        (return))
                      (:Is%20Not%20Valid
                        _)))
                  (:Is%20Not%20Valid
                    _))
                (return))
              (:Is%20Not%20Valid
                (return))))
          (:Is%20Not%20Valid
            (return)))))
    (:Is%20Not%20Valid
      (return))))