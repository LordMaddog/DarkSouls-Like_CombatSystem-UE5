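; BP_Beacon is a utility actor that shows a randomly colored beacon mesh which stretches upward when spawned.
; On BeginPlay, the TimeGrow timeline scales the static mesh's Z from 1 to 10.
; A dynamic material instance gets a random Color with channels well above 1, allowing overbright values.
; When ShouldSelfDelete is set, the actor destroys itself after Duration.
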(event Custom|Grow
  (bind _alpha (Timeline|TimeGrow PlayFromStart)
    (:Update
      (Transformation|SetWorldScale3D (Variables|Default|GetStaticMesh) (Math|Vector|MakeVector 1.0 1.0 (Math|Float|Lerp 1.0 1e+01 _alpha))))))

(event EventBeginPlay
  (bind _staticmesh (Variables|Default|GetStaticMesh))
  (CallFunction|Grow)
  (bind _returnvalue (Rendering|Material|CreateDynamicMaterialInstance _staticmesh 0 (Rendering|Material|GetMaterial _staticmesh 0) "None" :!class /Script/Engine.PrimitiveComponent))
  (Variables|Default|SetMat _returnvalue)
  (Rendering|Material|SetVectorParameterValue (Variables|Default|GetMat) "Color" (Utilities|Struct|MakeLinearColor (Math|Random|RandomFloatinRange 0.0 1e+02) (Math|Random|RandomFloatinRange 0.0 1e+02) (Math|Random|RandomFloatinRange 0.0 1e+02) 0.0) :!class /Script/Engine.MaterialInstanceDynamic)
  (if (Variables|Default|GetShouldSelfDelete)
    (Utilities|FlowControl|Delay (Variables|Default|GetDuration))
    (Actor|DestroyActor)))

(fn ConstructionScript)