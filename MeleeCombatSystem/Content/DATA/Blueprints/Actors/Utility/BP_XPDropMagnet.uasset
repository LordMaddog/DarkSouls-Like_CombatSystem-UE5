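; XP magnet pickup that activates the magnet effect on every BP_XPDrop in the level when collected.
; After BeginPlay delays it stops the mesh's physics and lifts it with a sweep.
; A sphere overlap passing ToCastOrNotToCast plays a sound once, calls XPMagnetActive on all drops, then destroys the actor.
; The construction script scales the Niagara sprite and ribbon by XPGiven, switching to a green system for high values.
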(event OnComponentBeginOverlap(Sphere)
  (params (OverlappedComponent :type Primitive%20Component%20Object%20Reference) (OtherActor :type Actor%20Object%20Reference) (OtherComp :type Primitive%20Component%20Object%20Reference) (OtherBodyIndex :type Integer) (bFromSweep :type Boolean) (SweepResult :type Hit%20Result%20Structure%20%28by%20ref%29))
  (bind _isplayer (CallFunction|ToCastorNottoCast OtherActor))
  (if _isplayer
    (Utilities|FlowControl|DoOnce false
      (:Completed
        (Audio|PlaySoundatLocation "/Game/DATA/SoundFX/XP/SC_XPMagnet.SC_XPMagnet" (Transformation|GetActorLocation) "0, 0, 0" 1.0 1.0 0.0 0 0 0 0)
        (bind _outactors (Actor|GetAllActorsOfClass "/Game/DATA/Blueprints/Actors/BP_XPDrop.BP_XPDrop_C"))
        (for _array_element _outactors
          (Default|XPMagnetActive _array_element))
        (Actor|DestroyActor)))))

(event EventBeginPlay
  ;[1 1 1] Start
  (|CallParentFunction)
  (Utilities|FlowControl|Delay 1.0)
  (Physics|SetSimulatePhysics (Variables|Default|GetDropMesh) false)
  (Utilities|FlowControl|Delay 0.5)
  (Transformation|SetWorldLocation (Variables|Default|GetDropMesh) (+ (Transformation|GetWorldLocation (Variables|Default|GetDropMesh)) "0.000000,0.000000,170.000000") true false))

(fn ConstructionScript
  (|CallParentFunction)
  (Effects|Components|ParticleSystem|SetFloatParameter (Variables|Default|GetN_Experience) "SpriteSize" (Math|Conversions|ToFloat(Integer) (+ (Variables|Default|GetXPGiven) 10)))
  (Effects|Components|ParticleSystem|SetFloatParameter (Variables|Default|GetN_Experience) "RibbonWidth" (+ (* (Variables|Default|GetXPGiven) 0.1) 2.0))
  (if (>= (Variables|Default|GetXPGiven) 20)
    (Class|NiagaraComponent|SetAsset (Variables|Default|GetN_Experience) "/Game/DATA/Effects/N_ExperienceParticelGreen.N_ExperienceParticelGreen" true)
    (Effects|Components|ParticleSystem|SetFloatParameter (Variables|Default|GetN_Experience) "SpriteSize" (+ (/ (Variables|Default|GetXPGiven) 10) 1e+01))
    (Effects|Components|ParticleSystem|SetFloatParameter (Variables|Default|GetN_Experience) "RibbonWidth" (+ (* (Variables|Default|GetXPGiven) 0.01) 2.0))))