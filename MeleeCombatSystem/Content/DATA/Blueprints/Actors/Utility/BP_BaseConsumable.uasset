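; Base class for consumable items, such as health potions, with a limited number of uses.
; On BeginPlay it fills the use count to its maximum and sends it to the player controller's potion amount display.
; The item action, while uses remain, asks the equipped combat component to perform the UseItem action with a montage.
; A separate ConsumeItem event decrements the count and updates that display with Visible set to false.
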(event Custom|ConsumeItem
  (bind _result (Math|Integer|DecrementInt (Variables|Default|GetCurrentNumberOfUses))
    (:%20%20
      (Class|CombatBPI|UpdateHealthPotionAmount(Message) (Game|GetPlayerController 0) _result false))))

(event EventBeginPlay
  (|CallParentFunction)
  (bind _output_get (Variables|Default|SetCurrentNumberOfUses (Variables|Default|GetMaxNumberOfUses)))
  (Class|CombatBPI|UpdateHealthPotionAmount(Message) (Game|GetPlayerController 0) _output_get true (Variables|Default|GetImage%20Style)))

(event Collision|EventActorBeginOverlap
  (params (OtherActor :type Actor%20Object%20Reference))
  (|CallParentFunction OtherActor) ; This node is disabled and will not be called.\nDrag off pins to build functionality.
)

(event EventTick
  (params (DeltaSeconds :type Float%20%28single-precision%29))
  (|CallParentFunction DeltaSeconds) ; This node is disabled and will not be called.\nDrag off pins to build functionality.
)

(event EventPreformItemAction
  (|CallParentFunction)
  (if (> (Variables|Default|GetCurrentNumberOfUses) 0)
    (bind _success_ (Class|CombatBPI|PreformCustomAction(Message) (Variables|Default|GetEquippedCombatComponent) "(TagName=\"Character.Action.UseItem\")" "(TagName=\"Character.State.GenralActionState\")" (Variables|Montages|GetUseItemMontage_0) 1.0 false))
    (if _success_
      _)))

(fn ConstructionScript
  (|CallParentFunction))