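; Base useable inventory item that puts the player into a build pawn to place an object of its placeable class.
; UseItem spawns a temporary BP_BuildPawn above the player, passes it the item info and class, and possesses it.
; It then turns off the mouse cursor, hides the hotbars, minimap and inventory, and destroys itself.
; A separate ConsumeUsedItem event decrements a player stat and also destroys the actor.
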(event EventBeginPlay
  (|CallParentFunction) ; This node is disabled and will not be called.\nDrag off pins to build functionality.
)

(event Collision|EventActorBeginOverlap
  (params (OtherActor :type Actor%20Object%20Reference)))

(event EventTick
  (params (DeltaSeconds :type Float%20%28single-precision%29)))

(event EventConsumeUsedItem
  (Default|ModifyCurrentStatValue (Variables|/Game/DATA/BP_PC.BP_PC_C|GetStatsComponent (Variables|/Game/DATA/Blueprints/Actors/Inventory/BP_Inventory.BP_Inventory_C|GetPlayer (Variables|Default|GetInventory))) "NewEnumerator5" -1.0 false)
  (Actor|DestroyActor))

(fn ConstructionScript
  (|CallParentFunction))

(fn UseItem
  (params (ItemInfo :type S%20Item%20Info%20Structure))
  (bind _inventory (Variables|Default|GetInventory))
  (bind _inventory_2 (Variables|Default|GetInventory))
  (bind _inventory_3 (Variables|Default|GetInventory))
  (bind (_itemname _description _canbeused _usetext _canbestatcked_ _category _itemicon) (Utilities|Struct|BreakS_ItemInfo (Variables|Default|GetItemInfo)))
  (bind _player (Variables|/Game/DATA/Blueprints/Actors/Inventory/BP_Inventory.BP_Inventory_C|GetPlayer _inventory_2))
  (bind _player_2 (Variables|/Game/DATA/Blueprints/Actors/Inventory/BP_Inventory.BP_Inventory_C|GetPlayer _inventory))
  (bind _player_3 (Variables|/Game/DATA/Blueprints/Actors/Inventory/BP_Inventory.BP_Inventory_C|GetPlayer _inventory_3))
  (bind _returnvalue (Transformation|GetActorTransform _player_3))
  (bind _player_controller (Variables|/Game/DATA/BP_PC.BP_PC_C|GetPlayer%20Controller _player_2))
  (bind _inventory_4 (Variables|/Game/DATA/BP_PC.BP_PC_C|GetInventory _player_2))
  ;[1 1 1] When Used this is what changed.
  (bind _returnvalue_2 (Game|SpawnActorfromClass "/Game/DATA/BP_BuildPawn.BP_BuildPawn_C" (Math|Transform|MakeTransform (+ (.location _returnvalue) "0.000000,0.000000,150.000000") (.rotation _returnvalue) (.scale _returnvalue)) "Undefined" "MultiplyWithRoot" _player _player true _player))
  ;;[1 1 1] Change Temp Info Class
  (Variables|/Game/DATA/BP_BuildPawn.BP_BuildPawn_C|SetTempInfo _returnvalue_2 (Utilities|Struct|MakeS_TempBuildInfo _itemicon _itemname _description (Utilities|Array|MakeArray _itemname) (Variables|ManualChangeVariables|GetPlacable%20Class)))
  (Pawn|Possess _player_controller _returnvalue_2)
  (Class|CombatBPI|SetMouseCursorActive(Message) _player_controller false)
  (Widget|SetVisibility (Variables|/Game/DATA/UI/Inventory/WBP_MainWidget.WBP_MainWidget_C|GetCW_AbilityHotKeyBar (Variables|/Game/DATA/Blueprints/Actors/Inventory/BP_Inventory.BP_Inventory_C|GetMainWidget _inventory_4)) "Collapsed")
  (Default|HideInventory _inventory_4)
  (Actor|DestroyActor))