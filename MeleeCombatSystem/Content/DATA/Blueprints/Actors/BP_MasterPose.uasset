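; BP_MasterPose is an equippable armor item whose skeletal mesh follows the owning character's animation.
; AttachActor snaps the item mesh to a socket on the character mesh, then sets that mesh as its leader pose component so both share one pose.
; OnEquipped and OnUnequipped extend the parent logic by adding and subtracting ArmorValue on a stat through EquippedStatComponent.
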(event EventBeginPlay
  (|CallParentFunction) ; This node is disabled and will not be called.\nDrag off pins to build functionality.
)

(event Collision|EventActorBeginOverlap
  (params (OtherActor :type Actor%20Object%20Reference))
  (|CallParentFunction OtherActor) ; This node is disabled and will not be called.\nDrag off pins to build functionality.
)

(event EventTick
  (params (DeltaSeconds :type Float%20%28single-precision%29))
  (|CallParentFunction DeltaSeconds) ; This node is disabled and will not be called.\nDrag off pins to build functionality.
)

(fn ConstructionScript
  (|CallParentFunction))

(fn AttachActor
  (params (SocketName :type Name :default "None") (LocationRule :type EAttachmentRule%20Enum :default "KeepRelative"))
  (bind _returnvalue (Components|GetOwner))
  (bind _ascharacter (Utilities|Casting|CastToCharacter _returnvalue))
  (bind _mesh (Variables|/Script/Engine.Character|GetMesh _ascharacter))
  (Utilities|IsValid (Variables|/Script/Engine.SkeletalMeshComponent|GetSkeletalMeshAsset (Variables|Default|GetItemSkeletalMesh))
    (:Is%20Valid
      (Transformation|AttachComponentToComponent (Variables|Default|GetItemSkeletalMesh) _mesh SocketName "SnapToTarget" "SnapToTarget" "SnapToTarget" true)
      (Components|SkinnedMesh|SetLeaderPoseComponent (Variables|Default|GetItemSkeletalMesh) _mesh true false))))

(fn OnEquipped
  (|CallParentFunction)
  (Variables|Default|GetEquippedStat%20Component
    (:then
      (Default|ModifyCurrentStatValue (Variables|Default|GetEquippedStat%20Component) "NewEnumerator3" (Variables|Stat|GetArmorValue) false))
    (:else)))

(fn OnUnequipped
  (|CallParentFunction)
  (Default|ModifyCurrentStatValue (Variables|Default|GetEquippedStat%20Component) "NewEnumerator3" (* (Variables|Stat|GetArmorValue) -1.0) false))