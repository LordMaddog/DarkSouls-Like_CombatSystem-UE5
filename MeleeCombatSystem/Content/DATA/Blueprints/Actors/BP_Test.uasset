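; BP_Test is a debug test actor for inspecting the position of its StaticMesh component.
; A GetData event prints the mesh's world location and its offset from the actor, computed as actor location minus mesh location.
; Leftover transform-conversion nodes sit unconnected in the graph, and BeginPlay and the construction script are empty.
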(event Custom|GetData
  (Development|PrintString (Utilities|String|Append "world:" (Utilities|String|ToString(Vector) (Transformation|GetWorldLocation (Variables|Default|GetStaticMesh)))))
  (Development|PrintString (Utilities|String|Append "Relitive:" (Utilities|String|ToString(Vector) (- (Transformation|GetActorLocation) (Transformation|GetWorldLocation (Variables|Default|GetStaticMesh)))))))

(event EventBeginPlay)

(fn ConstructionScript)