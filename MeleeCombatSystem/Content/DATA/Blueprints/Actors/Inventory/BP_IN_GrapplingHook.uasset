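; BP_IN_GrapplingHook is a single-use inventory item that gives the player a grappling hook ability.
; UseAbility reaches the player's CombatComponent through the Inventory reference, calls GrapplingCast with a fixed value, then destroys the item actor.
; The grapple logic lives in that component, and the event graph holds only disabled parent-call stubs.
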(event EventBeginPlay
  (|CallParentFunction) ; This node is disabled and will not be called.\nDrag off pins to build functionality.
)

(event Collision|EventActorBeginOverlap
  (params (OtherActor :type Actor%20Object%20Reference))
  (|CallParentFunction OtherActor) ; This node is disabled and will not be called.\nDrag off pins to build functionality.
)

(event EventTick
  (params (DeltaSeconds :type Float%20%28single-precision%29))
  (|CallParentFunction DeltaSeconds) ; This node is disabled and will not be called.\nDrag off pins to build functionality.
)

(fn ConstructionScript
  (|CallParentFunction))

(fn UseAbility
  (Default|GrapplingCast (Variables|/Game/DATA/BP_PC.BP_PC_C|GetCombatComponent (Variables|/Game/DATA/Blueprints/Actors/Inventory/BP_Inventory.BP_Inventory_C|GetPlayer (Variables|Default|GetInventory))) 6e+03)
  (Actor|DestroyActor))