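; Base inventory item actor that fills its info from an items data table row and handles being used by the player.
; On use it branches by category: armor and weapons go to the equipment component, consumables trigger a combat-component montage action, readables open a reading widget.
; Successful equips and ConsumeUsedItem remove one from the matching slot array and destroy the actor; OnRead destroys without removal.
; The Abilities branch is an empty stub.
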(event Custom|EventOnUsed
  (CallFunction|SelectUseType (.category (Variables|Initialize|GetItemInfo))))

(event Custom|ConsumeUsedItem
  (CallFunction|RemoveItematIndex)
  (Actor|DestroyActor))

(event EventBeginPlay
  (Utilities|FlowControl|Delay 1.0)
  (CallFunction|UpdateInfo))

(event Collision|EventActorBeginOverlap
  (params (OtherActor :type Actor%20Object%20Reference)))

(event EventTick
  (params (DeltaSeconds :type Float%20%28single-precision%29))
  (Utilities|FlowControl|DoOnce false
    (:Completed
      (CallFunction|UpdateInfo))))

(fn ConstructionScript
  (CallFunction|UpdateInfo))

(fn SelectUseType
  (params (Selection :type E_ItemCategories%20Enum :default "NewEnumerator0"))
  (switch Utilities|FlowControl|Switch|SwitchonE_ItemCategories Selection
    (:NewEnumerator0
      (CallFunction|EquipArmor))
    (:NewEnumerator1
      (CallFunction|UseItem))
    (:NewEnumerator4
      (CallFunction|ReadableItem))
    (:NewEnumerator2
      (CallFunction|EquipWeapon))
    (:NewEnumerator6
      (CallFunction|UseAbility))))

(fn EquipArmor
  (bind _success_ (Default|EquipItem (Actor|GetComponentbyClass (Variables|/Game/DATA/Blueprints/Actors/Inventory/BP_Inventory.BP_Inventory_C|GetPlayer (Variables|Initialize|GetInventory)) "/Game/DATA/Blueprints/Components/EquipmentComponet.EquipmentComponet_C") (.selfreff (Variables|Initialize|GetItemInfo)) "NewEnumerator7"))
  (if _success_
    (CallFunction|RemoveItematIndex)
    (Actor|DestroyActor)))

(fn EquipWeapon
  (bind _success_ (Default|EquipItem (Actor|GetComponentbyClass (Variables|/Game/DATA/Blueprints/Actors/Inventory/BP_Inventory.BP_Inventory_C|GetPlayer (Variables|Initialize|GetInventory)) "/Game/DATA/Blueprints/Components/EquipmentComponet.EquipmentComponet_C") (.selfreff (Variables|Initialize|GetItemInfo)) "NewEnumerator7"))
  (if _success_
    (CallFunction|RemoveItematIndex)
    (Actor|DestroyActor)))

(fn UseItem
  (Class|CombatBPI|PreformCustomAction(Message) (Variables|/Game/DATA/BP_PC.BP_PC_C|GetCombatComponent (Variables|/Game/DATA/Blueprints/Actors/Inventory/BP_Inventory.BP_Inventory_C|GetPlayer (Variables|Initialize|GetInventory))) "(TagName=\"Character.Action.UseItem\")" "(TagName=\"Character.State.GenralActionState\")" (Variables|Default|GetUseItemMontage) 1.0 false))

(fn ReadableItem
  (Utilities|FlowControl|DoOnce false
    (:Completed
      (Widget|SetIsEnabled (Variables|/Game/DATA/UI/Inventory/WBP_MainWidget.WBP_MainWidget_C|GetBPW_Inventory (Variables|/Game/DATA/Blueprints/Actors/Inventory/BP_Inventory.BP_Inventory_C|GetMainWidget (Variables|Initialize|GetInventory))) false)
      (bind _returnvalue (UserInterface|CreateWidget (Variables|Initialize|GetReadingItem) 0 self))
      (bind _output_get (Variables|Initialize|SetReadingWidget _returnvalue))
      (Widget|Panel|AddChild (Variables|/Game/DATA/UI/Inventory/WBP_MainWidget.WBP_MainWidget_C|GetCanvas (Variables|/Game/DATA/Blueprints/Actors/Inventory/BP_Inventory.BP_Inventory_C|GetMainWidget (Variables|Initialize|GetInventory))) _output_get)
      (Class|CanvasPanelSlot|SetAnchors (Class|WidgetLayoutLibrary|SlotasCanvasSlot (Variables|Initialize|GetReadingWidget)) (Utilities|Struct|MakeAnchors "(X=0.500000,Y=0.500000)" "(X=0.500000,Y=0.500000)"))
      (Class|CanvasPanelSlot|SetAutoSize (Class|WidgetLayoutLibrary|SlotasCanvasSlot (Variables|Initialize|GetReadingWidget)) true)
      (Class|CanvasPanelSlot|SetPosition (Class|WidgetLayoutLibrary|SlotasCanvasSlot (Variables|Initialize|GetReadingWidget)) "(X=-325.000000,Y=-240.000000)")
      (Input|SetInputModeUIOnly (Game|GetPlayerController 0) (Variables|Initialize|GetReadingWidget) "DoNotLock" false))))

(fn OnRead
  (Widget|SetIsEnabled (Variables|/Game/DATA/UI/Inventory/WBP_MainWidget.WBP_MainWidget_C|GetBPW_Inventory (Variables|/Game/DATA/Blueprints/Actors/Inventory/BP_Inventory.BP_Inventory_C|GetMainWidget (Variables|Initialize|GetInventory))) true)
  (Widget|RemovefromParent (Variables|Initialize|GetReadingWidget))
  (Input|SetInputModeGameandUI (Game|GetPlayerController 0) 0 "DoNotLock" false false)
  (Actor|DestroyActor))

(fn SetItem
  (params (RowName :type Name))
  (bind _returnvalue (Utilities|GetDataTableRow "/Game/DATA/Blueprints/DataTables/Table_InventoryItemsList.Table_InventoryItemsList" RowName)
    (:then
      (Variables|Initialize|SetItemInfo _returnvalue)
      (return))))

(fn GetSlotType
  (switch Utilities|FlowControl|Switch|SwitchonE_SlotTypes (Variables|Default|GetSlotType)
    (:NewEnumerator0
      (return 0))
    (:NewEnumerator1
      (return 1))
    (:NewEnumerator2
      (return 2))))

(fn RemoveItematIndex
  (bind _inventory (Variables|Initialize|GetInventory))
  (Default|RemoveItematIndexAlt (Variables|Initialize|GetInventory) (Variables|Initialize|GetIndex) 1 false (Utilities|Select :Index (CallFunction|GetSlotType) :Option%200 (Variables|/Game/DATA/Blueprints/Actors/Inventory/BP_Inventory.BP_Inventory_C|GetSlots _inventory) :Option%201 (Variables|/Game/DATA/Blueprints/Actors/Inventory/BP_Inventory.BP_Inventory_C|GetSlotsConsumables _inventory) :Option%202 (Variables|/Game/DATA/Blueprints/Actors/Inventory/BP_Inventory.BP_Inventory_C|GetSlotsSecondaryWeapons _inventory)))
  (return))

(fn UpdateInfo
  (bind _returnvalue (Utilities|GetDataTableRow "/Game/DATA/Blueprints/DataTables/Table_InventoryItemsList.Table_InventoryItemsList" (Variables|DataTable|GetItemNameDataTable))
    (:then
      (Variables|Initialize|SetItemInfo _returnvalue))))

(fn UseAbility)