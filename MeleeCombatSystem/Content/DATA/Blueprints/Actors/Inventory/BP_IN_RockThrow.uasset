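; BP_IN_RockThrow is an inventory item actor that gives the player a rock throw ability.
; UseAbility spawns a GA_PlayerRockThrow actor with the inventory's player as owner and instigator, sends it GAStartMessage, then destroys the item actor.
; The throw logic lives outside this Blueprint, whose construction script only calls its parent and whose standard events are disabled.
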(event EventBeginPlay
  (|CallParentFunction) ; This node is disabled and will not be called.\nDrag off pins to build functionality.
)

(event Collision|EventActorBeginOverlap
  (params (OtherActor :type Actor%20Object%20Reference))
  (|CallParentFunction OtherActor) ; This node is disabled and will not be called.\nDrag off pins to build functionality.
)

(event EventTick
  (params (DeltaSeconds :type Float%20%28single-precision%29))
  (|CallParentFunction DeltaSeconds) ; This node is disabled and will not be called.\nDrag off pins to build functionality.
)

(fn ConstructionScript
  (|CallParentFunction))

(fn UseAbility
  (bind _inventory (Variables|Default|GetInventory))
  (bind _player (Variables|/Game/DATA/Blueprints/Actors/Inventory/BP_Inventory.BP_Inventory_C|GetPlayer _inventory))
  (bind _returnvalue (Game|SpawnActorfromClass "/Game/DATA/Blueprints/Abilities/GA_PlayerRockThrow.GA_PlayerRockThrow_C" (Math|Transform|MakeTransform "0, 0, 0" "0, 0, 0" "1.000000,1.000000,1.000000") "Undefined" "MultiplyWithRoot" _player 0 _player))
  (Class|GamePlayAbilitiesBPI|GAStart(Message) _returnvalue)
  (Actor|DestroyActor))