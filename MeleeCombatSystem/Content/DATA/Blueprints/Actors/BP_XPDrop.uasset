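; BP_XPDrop is an experience pickup that flies toward the player and grants XP when collected.
; Within close range, or on PulltoPlayer, impulses pull its physics cube toward the player with a slight lift.
; Overlap or Interact triggers a one-time collection, adding XP scaled by a player sub-stat, playing a sound and destroying the actor.
; The construction script sizes the Niagara effect by XP amount and swaps to a green effect for larger drops.
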(event OnComponentBeginOverlap(Sphere)
  (params (OverlappedComponent :type Primitive%20Component%20Object%20Reference) (OtherActor :type Actor%20Object%20Reference) (OtherComp :type Primitive%20Component%20Object%20Reference) (OtherBodyIndex :type Integer) (bFromSweep :type Boolean) (SweepResult :type Hit%20Result%20Structure%20%28by%20ref%29))
  (bind _character (Variables|Default|GetCharacter))
  (bind _statscomponent (Variables|/Game/DATA/BP_PC.BP_PC_C|GetStatsComponent _character))
  ;[1 1 1] Give XP and delete self
  (if (== OtherActor (Game|GetPlayerCharacter 0))
    (Utilities|FlowControl|DoOnce false
      (:Completed
        (Components|Activation|Activate (Variables|Default|GetParticleSystem) true)
        (Utilities|FlowControl|Delay 0.1)
        (Utilities|IsValid _statscomponent
          (:Is%20Valid
            (Default|ModifyXP _statscomponent "NewEnumerator0" (Math|Float|Truncate (* (Variables|Default|GetXPGiven) (Default|GetSubStats (Variables|/Game/DATA/BP_PC.BP_PC_C|GetStatsComponent (Variables|Default|GetCharacter)) "NewEnumerator20"))))
            (Audio|PlaySoundatLocation "/Game/DATA/SoundFX/XP/SC_Xp.SC_Xp" (Transformation|GetActorLocation) "0, 0, 0" 1.0 1.0 0.0 0 0 0 0)
            (Actor|DestroyActor)))))))

(event EventBeginPlay
  ;[1 1 1] Start
  (bind _asbp_pc (Utilities|Casting|CastToBP_PC (Game|GetPlayerCharacter 0)))
  (Variables|Default|SetCharacter _asbp_pc))

(event EventPulltoPlayer
  (params (Actor :type Vector :default "0, 0, 0"))
  ;[1 1 1] Pull XP
  (Physics|AddImpulse (Variables|Default|GetCube) (+ (* (Math|Vector|GetForwardVector (Math|Rotator|FindLookatRotation (Transformation|GetWorldLocation (Variables|Default|GetCube)) (Transformation|GetActorLocation (Variables|Default|GetCharacter)))) (Variables|Default|GetPullPower)) "0.000000,0.000000,4.000000") "None" true))

(event EventTick
  (params (DeltaSeconds :type Float%20%28single-precision%29))
  ;[1 1 1] Pull XP
  (if (<= (Math|Vector|Distance(Vector) (Transformation|GetWorldLocation (Variables|Default|GetCube)) (Transformation|GetActorLocation (Variables|Default|GetCharacter))) 4e+02)
    (Physics|AddImpulse (Variables|Default|GetCube) (+ (* (Math|Vector|GetForwardVector (Math|Rotator|FindLookatRotation (Transformation|GetWorldLocation (Variables|Default|GetCube)) (Transformation|GetActorLocation (Variables|Default|GetCharacter)))) (Variables|Default|GetPullPower)) "0.000000,0.000000,4.000000") "None" true)))

(event EventInteract
  (params (CallEvent :type Actor%20Object%20Reference))
  (bind _character (Variables|Default|GetCharacter))
  (bind _statscomponent (Variables|/Game/DATA/BP_PC.BP_PC_C|GetStatsComponent _character))
  ;[1 1 1] Give XP and delete self
  (Utilities|FlowControl|DoOnce false
    (:Completed
      (Components|Activation|Activate (Variables|Default|GetParticleSystem) true)
      (Utilities|FlowControl|Delay 0.1)
      (Utilities|IsValid _statscomponent
        (:Is%20Valid
          (Default|ModifyXP _statscomponent "NewEnumerator0" (Math|Float|Truncate (* (Variables|Default|GetXPGiven) (Default|GetSubStats (Variables|/Game/DATA/BP_PC.BP_PC_C|GetStatsComponent (Variables|Default|GetCharacter)) "NewEnumerator20"))))
          (Audio|PlaySoundatLocation "/Game/DATA/SoundFX/XP/SC_Xp.SC_Xp" (Transformation|GetActorLocation) "0, 0, 0" 1.0 1.0 0.0 0 0 0 0)
          (Actor|DestroyActor))))))

(fn ConstructionScript
  (|CallParentFunction)
  (Effects|Components|ParticleSystem|SetFloatParameter (Variables|Default|GetN_Experience) "SpriteSize" (Math|Conversions|ToFloat(Integer) (+ (Variables|Default|GetXPGiven) (+ 10 0))))
  (Effects|Components|ParticleSystem|SetFloatParameter (Variables|Default|GetN_Experience) "RibbonWidth" (+ (+ 2 0) (* (Variables|Default|GetXPGiven) 0.1)))
  (if (>= (Variables|Default|GetXPGiven) 20)
    (Class|NiagaraComponent|SetAsset (Variables|Default|GetN_Experience) "/Game/DATA/Effects/N_ExperienceParticelGreen.N_ExperienceParticelGreen" true)
    (Effects|Components|ParticleSystem|SetFloatParameter (Variables|Default|GetN_Experience) "SpriteSize" (+ (+ 1e+01 0.0) (/ (Variables|Default|GetXPGiven) 10)))
    (Effects|Components|ParticleSystem|SetFloatParameter (Variables|Default|GetN_Experience) "RibbonWidth" (+ (+ 2 0) (* (Variables|Default|GetXPGiven) 0.01)))))