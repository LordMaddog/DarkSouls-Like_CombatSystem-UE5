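; BP_PickUpActor is a world pickup that gives its Item to the actor that interacts with it.
; Interact passes Item to that actor's EquipmentComponet via EquipItem, activates the particle system, then immediately destroys the pickup.
; PulltoPlayer launches the Cube component toward a given actor with a mass-independent impulse scaled by PullPower, plus a small upward lift.
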(event EventPulltoPlayer
  (params (Actor :type Vector :default "0, 0, 0"))
  (Physics|AddImpulse (Variables|Default|GetCube) (+ (* (Math|Vector|GetForwardVector (Math|Rotator|FindLookatRotation (Transformation|GetWorldLocation (Variables|Default|GetCube)) Actor)) (Variables|Default|GetPullPower)) "0.000000,0.000000,8.000000") "None" true))

(event EventInteract
  (params (CallEvent :type Actor%20Object%20Reference))
  (Default|EquipItem (Actor|GetComponentbyClass CallEvent "/Game/DATA/Blueprints/Components/EquipmentComponet.EquipmentComponet_C") (Variables|Default|GetItem))
  (Components|Activation|Activate (Variables|Default|GetParticleSystem) false)
  (Actor|DestroyActor))

(fn ConstructionScript)