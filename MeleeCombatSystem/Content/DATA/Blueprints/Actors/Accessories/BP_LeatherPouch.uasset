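; Leather pouch accessory Blueprint that attaches itself to the equipping character's mesh in one of four accessory slots.
; On equip it copies the desired equip type, then selects that slot's socket name and stored transform.
; AttachAccessory attaches the item's static mesh, or skeletal mesh as fallback, to the socket and applies the relative transform.
; SaveCurrentTrans records the mesh's current relative transform.
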(event Custom|AccessoryEquipped
  (switch Utilities|FlowControl|Switch|SwitchonE_EquipType (Variables|Default|GetEquipType)
    (:NewEnumerator15
      (CallFunction|AttachAccessory (Variables|Accessory|GetAccessoryOneSocket%20Name) (Variables|Accessory|GetAccessoryOneTrans)))
    (:NewEnumerator16
      (CallFunction|AttachAccessory (Variables|Accessory|GetAccessoryTwoSocket%20Name) (Variables|Accessory|GetAccessoryTwoTrans)))
    (:NewEnumerator17
      (CallFunction|AttachAccessory (Variables|Accessory|GetAccessoryThreeSocket%20Name) (Variables|Accessory|GetAccessoryThreeTrans)))
    (:NewEnumerator18
      (CallFunction|AttachAccessory (Variables|Accessory|GetAccessoryFourSocket%20Name) (Variables|Accessory|GetAccessoryFourTrans)))))

(event Custom|SaveCurrentTrans
  (Variables|Default|SetCurrentTransform (Transformation|GetRelativeTransform (CallFunction|GetMesh))))

(event EventBeginPlay
  (|CallParentFunction) ; This node is disabled and will not be called.\nDrag off pins to build functionality.
)

(event Collision|EventActorBeginOverlap
  (params (OtherActor :type Actor%20Object%20Reference))
  (|CallParentFunction OtherActor) ; This node is disabled and will not be called.\nDrag off pins to build functionality.
)

(event EventTick
  (params (DeltaSeconds :type Float%20%28single-precision%29))
  (|CallParentFunction DeltaSeconds) ; This node is disabled and will not be called.\nDrag off pins to build functionality.
)

(fn ConstructionScript
  (|CallParentFunction))

(fn OnEquipped
  (|CallParentFunction)
  (Variables|Default|SetEquipType (Variables|Default|GetDesiredEquipType))
  (CallFunction|AccessoryEquipped))

(fn GetMesh
  (Utilities|IsValid (Variables|Default|GetItemStaticMesh)
    (:Is%20Valid
      (return (Variables|Default|GetItemStaticMesh)))
    (:Is%20Not%20Valid
      (Utilities|IsValid (Variables|Default|GetItemSkeletalMesh)
        (:Is%20Valid
          (return (Variables|Default|GetItemSkeletalMesh)))))))

(fn AttachAccessory
  (params (SocketName :type Name) (NewTransform :type Transform%20%28by%20ref%29))
  (bind _attachrule (Variables|Default|GetAttachRule))
  (Transformation|AttachComponentToComponent (CallFunction|GetMesh) (Variables|/Script/Engine.Character|GetMesh (Variables|Default|GetEquipped%20Character)) SocketName _attachrule _attachrule _attachrule true)
  (Transformation|SetRelativeTransform (CallFunction|GetMesh) NewTransform false true))