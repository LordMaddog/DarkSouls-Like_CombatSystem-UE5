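; BP_Necklace is an equippable necklace accessory that attaches to the character wearing it.
; On equip, it runs the parent logic, then adopts the desired equip type if it matches one of four allowed slots.
; It attaches its skeletal mesh to a socket on the character mesh and applies a fixed relative offset and rotation.
; Physical animation setup exists but is disconnected, and the event graph is empty.
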(event EventBeginPlay
  (|CallParentFunction) ; This node is disabled and will not be called.\nDrag off pins to build functionality.
)

(event Collision|EventActorBeginOverlap
  (params (OtherActor :type Actor%20Object%20Reference))
  (|CallParentFunction OtherActor) ; This node is disabled and will not be called.\nDrag off pins to build functionality.
)

(event EventTick
  (params (DeltaSeconds :type Float%20%28single-precision%29))
  (|CallParentFunction DeltaSeconds) ; This node is disabled and will not be called.\nDrag off pins to build functionality.
)

(fn ConstructionScript
  (|CallParentFunction))

(fn OnEquipped
  (bind _attachrule (Variables|Default|GetAttachRule))
  (bind _desiredequiptype (Variables|Default|GetDesiredEquipType))
  (|CallParentFunction)
  (if (not (Math|Boolean|ORBoolean (Utilities|Enum|Equal(Enum) _desiredequiptype "NewEnumerator15") (Utilities|Enum|Equal(Enum) _desiredequiptype "NewEnumerator16") (Utilities|Enum|Equal(Enum) _desiredequiptype "NewEnumerator17") (Utilities|Enum|Equal(Enum) _desiredequiptype "NewEnumerator18")))
    _
    (else
      (Variables|Default|SetEquipType (Variables|Default|GetDesiredEquipType))))
  (Transformation|AttachComponentToComponent (Variables|Default|GetItemSkeletalMesh) (Variables|/Script/Engine.Character|GetMesh (Variables|Default|GetEquipped%20Character)) (Variables|Default|GetAttachSocket%20Name) _attachrule _attachrule _attachrule true)
  (Transformation|SetRelativeLocationAndRotation (Variables|Default|GetItemSkeletalMesh) "30.000000,3.000000,0.000000" "-90.000000,0.000000,0.000000" false true))