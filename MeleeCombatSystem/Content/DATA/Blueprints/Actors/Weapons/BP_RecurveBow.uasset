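; BP_RecurveBow is a recurve bow weapon Blueprint that layers small overrides on inherited weapon behavior.
; On equip it runs the parent logic, then sets itself two-handed if there is no off-hand weapon.
; Collision activation and deactivation switch the swing sound between a sword swing and a bow release before calling the parent, so melee hits and shots share one sound component.
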(event EventBeginPlay
  (|CallParentFunction))

(event Collision|EventActorBeginOverlap
  (params (OtherActor :type Actor%20Object%20Reference))
  (|CallParentFunction OtherActor) ; This node is disabled and will not be called.\nDrag off pins to build functionality.
)

(event EventTick
  (params (DeltaSeconds :type Float%20%28single-precision%29))
  (|CallParentFunction DeltaSeconds) ; This node is disabled and will not be called.\nDrag off pins to build functionality.
)

(fn ConstructionScript
  (|CallParentFunction))

(fn OnEquipped
  (|CallParentFunction)
  (if (not (Variables|Default|GetOffHandWeapon))
    (CallFunction|SetTwoHanded true)))

(fn ActivateCollision
  (params (CollisionPart :type E_CollisionPart%20Enum :default "NewEnumerator0") (MagicLeft :type Boolean))
  (Audio|Components|Audio|SetSound (Variables|Default|GetSwingSound) "/Game/DATA/SoundFX/Weapon/SwordSwing.SwordSwing")
  (|CallParentFunction CollisionPart MagicLeft))

(fn DeactivateCollision
  (params (CollisionPart :type E_CollisionPart%20Enum :default "NewEnumerator0"))
  (Audio|Components|Audio|SetSound (Variables|Default|GetSwingSound) "/Game/DATA/SoundFX/Weapon/BowAndArrow/SC_BowReleas.SC_BowReleas")
  (|CallParentFunction CollisionPart))