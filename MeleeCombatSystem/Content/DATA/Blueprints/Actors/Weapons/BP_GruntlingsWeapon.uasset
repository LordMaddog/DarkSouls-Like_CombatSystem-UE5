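; BP_GruntlingsWeapon is a Gruntling weapon actor that picks a random look when play begins.
; After the parent BeginPlay, a random integer selects one of three static meshes for the GruntlingWeapon component, with Weapon03 weighted to three of the five outcomes.
; The overlap and tick events are disabled, and the construction script only calls its parent.
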(event EventBeginPlay
  (|CallParentFunction)
  (switch int (Math|Random|RandomIntegerinRange 0 4)
    (:0
      (Components|StaticMesh|SetStaticMesh (Variables|Default|GetGruntlingWeapon) "/Game/InfinityBladeAdversaries/Enemy/Enemy_Gruntling_Weapons/Meshes/SM_Creature_Gruntling_Weapon03_Internal.SM_Creature_Gruntling_Weapon03_Internal"))
    (:1
      (Components|StaticMesh|SetStaticMesh (Variables|Default|GetGruntlingWeapon) "/Game/InfinityBladeAdversaries/Enemy/Enemy_Gruntling_Weapons/Meshes/SM_Creature_Gruntling_Weapon03_Internal.SM_Creature_Gruntling_Weapon03_Internal"))
    (:2
      (Components|StaticMesh|SetStaticMesh (Variables|Default|GetGruntlingWeapon) "/Game/InfinityBladeAdversaries/Enemy/Enemy_Gruntling_Weapons/Meshes/SM_Creature_Gruntling_Weapon03_Internal.SM_Creature_Gruntling_Weapon03_Internal"))
    (:3
      (Components|StaticMesh|SetStaticMesh (Variables|Default|GetGruntlingWeapon) "/Game/InfinityBladeAdversaries/Enemy/Enemy_Gruntling_Weapons/Meshes/SM_Gruntling_Weapon01_Internal.SM_Gruntling_Weapon01_Internal"))
    (:4
      (Components|StaticMesh|SetStaticMesh (Variables|Default|GetGruntlingWeapon) "/Game/InfinityBladeAdversaries/Enemy/Enemy_Gruntling_Weapons/Meshes/SM_Gruntling_Weapon02_Internal.SM_Gruntling_Weapon02_Internal"))))

(event Collision|EventActorBeginOverlap
  (params (OtherActor :type Actor%20Object%20Reference))
  (|CallParentFunction OtherActor) ; This node is disabled and will not be called.\nDrag off pins to build functionality.
)

(event EventTick
  (params (DeltaSeconds :type Float%20%28single-precision%29))
  (|CallParentFunction DeltaSeconds) ; This node is disabled and will not be called.\nDrag off pins to build functionality.
)

(fn ConstructionScript
  (|CallParentFunction))