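; BP_BaseCrossBow is the base crossbow weapon Blueprint, layering crossbow-specific behavior on a parent weapon class.
; Equipping marks it two-handed, and unequipping destroys any valid notched arrow.
; The CrossBowLoaded event sets the Loaded flag, and the IsStrafing? function always returns false.
; Construction only calls the parent, and BeginPlay, overlap and Tick are disabled.
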(event EventBeginPlay
  (|CallParentFunction) ; This node is disabled and will not be called.\nDrag off pins to build functionality.
)

(event Collision|EventActorBeginOverlap
  (params (OtherActor :type Actor%20Object%20Reference))
  (|CallParentFunction OtherActor) ; This node is disabled and will not be called.\nDrag off pins to build functionality.
)

(event EventTick
  (params (DeltaSeconds :type Float%20%28single-precision%29))
  (|CallParentFunction DeltaSeconds) ; This node is disabled and will not be called.\nDrag off pins to build functionality.
)

(event EventCrossBowLoaded
  (params (Vlaue :type Boolean))
  (Variables|Default|SetLoaded Vlaue))

(fn ConstructionScript
  (|CallParentFunction))

(fn OnEquipped
  (|CallParentFunction)
  (CallFunction|SetTwoHanded true))

(fn OnUnequipped
  (params (GiveBack? :type Boolean) (ForceDrop :type Boolean) (ItemInfoIn :type S%20Item%20Info%20Structure))
  (|CallParentFunction GiveBack? ForceDrop ItemInfoIn)
  (bind _notchedarrow (Variables|Default|GetNotchedArrow)
    (:then
      (Actor|DestroyActor _notchedarrow))
    (:else)))

(fn IsStrafing?
  (return false))