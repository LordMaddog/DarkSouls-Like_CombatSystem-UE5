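; BP_testChest is a test chest actor that the player can interact with to open an inventory UI.
; Its InteractComponent starts with prompt text, and the Sphere overlap events add or remove the chest from the interact list for qualifying actors.
; A valid Interact call passes the component's Player to the InventoryComponent and opens its UI.
; GetItemInfo is an empty stub.
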(event OnComponentBeginOverlap(Sphere)
  (params (OverlappedComponent :type Primitive%20Component%20Object%20Reference) (OtherActor :type Actor%20Object%20Reference) (OtherComp :type Primitive%20Component%20Object%20Reference) (OtherBodyIndex :type Integer) (bFromSweep :type Boolean) (SweepResult :type Hit%20Result%20Structure%20%28by%20ref%29))
  (bind _isplayer (Default|ToCastorNottoCast (Variables|Default|GetInteractComponent) OtherActor))
  (if _isplayer
    (Default|AddtoInteractList (Variables|Default|GetInteractComponent))))

(event OnComponentEndOverlap(Sphere)
  (params (OverlappedComponent :type Primitive%20Component%20Object%20Reference) (OtherActor :type Actor%20Object%20Reference) (OtherComp :type Primitive%20Component%20Object%20Reference) (OtherBodyIndex :type Integer))
  (bind _isplayer (Default|ToCastorNottoCast (Variables|Default|GetInteractComponent) OtherActor))
  (if _isplayer
    (Default|RemovefromInteractList (Variables|Default|GetInteractComponent))))

(event EventBeginPlay
  (Default|Start (Variables|Default|GetInteractComponent) self (Variables|Default|GetPickUpText) "oppen" "(R=1.000000,G=1.000000,B=1.000000,A=1.000000)"))

(event EventInteract
  (params (CallEvent :type Actor%20Object%20Reference))
  (bind _interactcomponent (Variables|Default|GetInteractComponent))
  (bind _returnvalue (Default|PInteract _interactcomponent CallEvent))
  (if _returnvalue
    (Default|SetPlayer (Variables|Default|GetInventoryComponent) (Variables|/Game/DATA/Blueprints/Components/InteractComponent.InteractComponent_C|GetPlayer _interactcomponent))
    (Default|OppenUI (Variables|Default|GetInventoryComponent))))

(fn ConstructionScript)

(fn GetItemInfo
  (return 0))