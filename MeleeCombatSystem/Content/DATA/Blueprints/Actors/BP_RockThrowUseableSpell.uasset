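; BP_RockThrowUseableSpell is a useable spell item that triggers the player's rock throw ability.
; Its UseAbility restarts the active GA_PlayerRockThrow on the player's CombatComponent, or clears the current ability, spawns a new one, starts it and registers it.
; Either way the item destroys itself afterward.
; UseAbility is marked deprecated, since the inventory now handles this through the GA set in the item info skill struct.
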(event EventBeginPlay
  (|CallParentFunction) ; This node is disabled and will not be called.\nDrag off pins to build functionality.
)

(event Collision|EventActorBeginOverlap
  (params (OtherActor :type Actor%20Object%20Reference)))

(event EventTick
  (params (DeltaSeconds :type Float%20%28single-precision%29)))

(fn ConstructionScript
  (|CallParentFunction))

(fn UseAbility
  (bind _inventory (Variables|Default|GetInventory))
  (bind _inventory_2 (Variables|Default|GetInventory))
  (bind _player (Variables|/Game/DATA/Blueprints/Actors/Inventory/BP_Inventory.BP_Inventory_C|GetPlayer _inventory))
  (bind _player_2 (Variables|/Game/DATA/Blueprints/Actors/Inventory/BP_Inventory.BP_Inventory_C|GetPlayer _inventory_2))
  (bind _combatcomponent (Variables|/Game/DATA/BP_PC.BP_PC_C|GetCombatComponent _player_2))
  (bind (_activega _returnvalue) (Default|IsGAActive _combatcomponent "/Game/DATA/Blueprints/Abilities/GA_PlayerRockThrow.GA_PlayerRockThrow_C"))
  ;[1 1 1] This is depricated. (now happens in the inventory it's self and GA is set in item info skill struct)
  (if _returnvalue
    (Class|GamePlayAbilitiesBPI|GAStart(Message) _activega)
    (Actor|DestroyActor)
    (else
      (Default|ClearGA _combatcomponent)
      (bind _returnvalue_2 (Game|SpawnActorfromClass "/Game/DATA/Blueprints/Abilities/GA_PlayerRockThrow.GA_PlayerRockThrow_C" (Math|Transform|MakeTransform "0, 0, 0" "0, 0, 0" "1.000000,1.000000,1.000000") "Undefined" "MultiplyWithRoot" _player 0 _player))
      (Class|GamePlayAbilitiesBPI|GAStart(Message) _returnvalue_2)
      (Default|AddGA (Variables|/Game/DATA/BP_PC.BP_PC_C|GetCombatComponent (Variables|/Game/DATA/Blueprints/Actors/Inventory/BP_Inventory.BP_Inventory_C|GetPlayer (Variables|Default|GetInventory))) "/Game/DATA/Blueprints/Abilities/GA_PlayerRockThrow.GA_PlayerRockThrow_C" _returnvalue_2)
      (Actor|DestroyActor))))