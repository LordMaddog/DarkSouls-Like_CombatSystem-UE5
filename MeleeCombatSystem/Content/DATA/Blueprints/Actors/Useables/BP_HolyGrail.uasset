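; BP_HolyGrail is a usable item actor that spends one point of a player stat when consumed.
; UseItem skips the parent logic and, if that stat is at least one, asks the player's CombatComponent to play the use-item montage as a custom action.
; The separate ConsumeUsedItem event lowers the stat through the StatsComponent without starting regeneration, then destroys the actor.
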(event EventBeginPlay
  (|CallParentFunction) ; This node is disabled and will not be called.\nDrag off pins to build functionality.
)

(event Collision|EventActorBeginOverlap
  (params (OtherActor :type Actor%20Object%20Reference)))

(event EventTick
  (params (DeltaSeconds :type Float%20%28single-precision%29)))

(event EventConsumeUsedItem
  (Default|ModifyCurrentStatValue (Variables|/Game/DATA/BP_PC.BP_PC_C|GetStatsComponent (Variables|/Game/DATA/Blueprints/Actors/Inventory/BP_Inventory.BP_Inventory_C|GetPlayer (Variables|Default|GetInventory))) "NewEnumerator5" -1.0 false)
  (Actor|DestroyActor))

(fn ConstructionScript
  (|CallParentFunction))

(fn UseItem
  (params (ItemInfo :type S%20Item%20Info%20Structure))
  (if (>= (Default|GetCurrentStatValue (Variables|/Game/DATA/BP_PC.BP_PC_C|GetStatsComponent (Variables|/Game/DATA/Blueprints/Actors/Inventory/BP_Inventory.BP_Inventory_C|GetPlayer (Variables|Default|GetInventory))) "NewEnumerator5") 1.0)
    (Class|CombatBPI|PreformCustomAction(Message) (Variables|/Game/DATA/BP_PC.BP_PC_C|GetCombatComponent (Variables|/Game/DATA/Blueprints/Actors/Inventory/BP_Inventory.BP_Inventory_C|GetPlayer (Variables|Default|GetInventory))) "(TagName=\"Character.Action.UseItem\")" "(TagName=\"Character.State.GenralActionState\")" (Variables|Default|GetUseItemMontage) 1.0 false)))