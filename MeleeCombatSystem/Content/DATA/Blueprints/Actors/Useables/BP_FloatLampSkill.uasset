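; Equippable floating lamp magic skill that attaches a Niagara light at a randomized offset beside the character and removes it with the equip mesh.
; On equip, a self-recursive delay loop grants FloatingLamp skill XP periodically.
; After a short delay, it registers the skill's mana cost in the visual stat buffs if absent, then drives light brightness, radius and mesh scale from skill Power and Effectiveness.
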(event Custom|SetLightBrightness
  (params (Brightness :type Float%20%28single-precision%29) (Radius :type Float%20%28single-precision%29))
  (Niagara|SetNiagaraVariable(Float) (Variables|Default|GetN_FloatingLamp) "LightBrightnessScale" Brightness)
  (Niagara|SetNiagaraVariable(Float) (Variables|Default|GetN_FloatingLamp) "LightRadiusScale" Radius)
  (Niagara|SetNiagaraVariable(Float) (Variables|Default|GetN_FloatingLamp) "MeshScale" (+ Radius Brightness)))

(event Custom|LevelUPTick
  (Utilities|FlowControl|Delay 1e+01)
  (Default|ModifySkillXP (Variables|/Game/DATA/BP_PC.BP_PC_C|GetStatsComponent (Variables|Default|GetEquipped%20Character)) "(TagName=\"Character.Action.Skill/Magic.FloatingLamp\")" 10 true)
  (CallFunction|LevelUPTick))

(event Custom|HasDebuff
  (bind _equipped_character (Variables|Default|GetEquipped%20Character))
  (bind _statscomponent (Variables|/Game/DATA/BP_PC.BP_PC_C|GetStatsComponent _equipped_character))
  (bind (_combat_types _mana_cost _stamina_cost _skill_xp _level_up_cost _skill_xpspent _skill_level _available_points _power _effectiveness) (Default|GetSkillStats _statscomponent "(TagName=\"Character.Action.Skill/Magic.FloatingLamp\")"))
  (Utilities|FlowControl|Delay 1.2)
  (if (not (.ReturnValue (Utilities|Map|Find (Variables|Default|GetVisualStatsBuff) "NewEnumerator8")))
    (Utilities|Map|Add (Variables|Default|GetVisualStatsBuff) "NewEnumerator8" (Math|Conversions|ToFloat(Integer) _mana_cost))
    (CallFunction|EquipedBuffStats)
    (CallFunction|SetLightBrightness (* _power 0.1) (* _effectiveness 0.1))))

(event EventBeginPlay
  (|CallParentFunction))

(event Collision|EventActorBeginOverlap
  (params (OtherActor :type Actor%20Object%20Reference))
  (|CallParentFunction OtherActor) ; This node is disabled and will not be called.\nDrag off pins to build functionality.
)

(event EventTick
  (params (DeltaSeconds :type Float%20%28single-precision%29))
  (|CallParentFunction DeltaSeconds))

(fn ConstructionScript
  (|CallParentFunction))

(fn RemoveEquipMesh
  (bind _n_floatinglamp (Variables|Default|GetN_FloatingLamp))
  (|CallParentFunction)
  (Utilities|IsValid _n_floatinglamp
    (:Is%20Valid
      (Components|DestroyComponent _n_floatinglamp))))

(fn SetRandomLoc
  (params (Target :type Scene%20Component%20Object%20Reference))
  (Transformation|SetRelativeLocation Target (Math|Vector|MakeVector (.x (Variables|/Script/Engine.SceneComponent|GetRelativeLocation Target)) (Math|Random|RandomFloatinRange -2.5e+02 -1e+02) (Math|Random|RandomFloatinRange -3e+01 6e+01)) false true))

(fn OnEquipped
  (Variables|Default|SetEquipType (Variables|Default|GetDesiredEquipType))
  (|CallParentFunction)
  (CallFunction|SetRandomLoc (Variables|Default|GetN_FloatingLamp))
  (CallFunction|LevelUPTick)
  (CallFunction|HasDebuff))