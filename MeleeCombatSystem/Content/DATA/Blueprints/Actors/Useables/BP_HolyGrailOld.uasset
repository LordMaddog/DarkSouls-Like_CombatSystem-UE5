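; BP_HolyGrailOld is a usable Holy Grail item that spends one point of a character stat per use.
; Using it checks that the stat is at least one, then asks the equipped combat component to play the use-item montage as a tagged action.
; A separate ConsumeItem event deducts the point without starting regeneration.
; On BeginPlay it sends the player controller a message hiding the health potion count.
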(event EventBeginPlay
  (|CallParentFunction)
  (Class|CombatBPI|UpdateHealthPotionAmount(Message) (Game|GetPlayerController 0) 0 false))

(event Collision|EventActorBeginOverlap
  (params (OtherActor :type Actor%20Object%20Reference))
  (|CallParentFunction OtherActor) ; This node is disabled and will not be called.\nDrag off pins to build functionality.
)

(event EventTick
  (params (DeltaSeconds :type Float%20%28single-precision%29))
  (|CallParentFunction DeltaSeconds) ; This node is disabled and will not be called.\nDrag off pins to build functionality.
)

(event EventConsumeItem
  (Default|ModifyCurrentStatValue (Variables|/Game/DATA/BP_PC.BP_PC_C|GetStatsComponent (Variables|Default|GetEquipped%20Character)) "NewEnumerator5" -1.0 false))

(event EventPreformItemAction
  (if (>= (Default|GetCurrentStatValue (Variables|/Game/DATA/BP_PC.BP_PC_C|GetStatsComponent (Variables|Default|GetEquipped%20Character)) "NewEnumerator5") 1.0)
    (Class|CombatBPI|PreformCustomAction(Message) (Variables|Default|GetEquippedCombatComponent) "(TagName=\"Character.Action.UseItem\")" "(TagName=\"Character.State.GenralActionState\")" (Variables|Default|GetUseItemMontage_0) 1.0 false)))

(fn ConstructionScript
  (|CallParentFunction))