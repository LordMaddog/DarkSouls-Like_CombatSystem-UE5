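; Ice crystal useable item whose floating Niagara crystal reflects the equipped owner's Water stat and regenerates it.
; On equip it binds to stat updates, scaling and repositioning the crystal as Water changes, with a timeline easing growth.
; A looping timer adds buff-scaled Water and skill XP, and stops once Water is full.
; Events toggle a pull force and sound for spells; UseAbility is deprecated in favor of inventory-driven abilities.
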(event Custom|DeactivatePullEffect
  ;[1 1 1] Spell pull effect activate/Deactivate
  (Niagara|SetNiagaraVariable(Float) (Variables|Default|GetN_FloatingCrystal) "PullForce" 0.0)
  (Audio|Components|Audio|Stop (Variables|Default|GetPullSound)))

(event Custom|ActivatePullEffect
  ;[1 1 1] Spell pull effect activate/Deactivate
  (Niagara|SetNiagaraVariable(Float) (Variables|Default|GetN_FloatingCrystal) "PullForce" 2e+02)
  (Audio|Components|Audio|Play (Variables|Default|GetPullSound) 0.0))

(event Custom|Update%20Water
  (params (StatsType :type E_SubStats%20Enum :default "NewEnumerator9") (Value :type Float%20%28double-precision%29))
  ;[1 1 1] Crystal Size. (Called on water update through binding in stat comp)
  (switch Utilities|FlowControl|Switch|SwitchonE_SubStats StatsType
    (:NewEnumerator37
      (if (!= (Class|KismetMathLibrary|FTrunc64 (* (Variables|Default|GetCurrentCrystal%20size) 0.8)) (Default|GetSubStats (Variables|Default|GetEquippedStat%20Component) "NewEnumerator37"))
        (CallFunction|CheckTimer)
        (if (> Value (Variables|Default|GetCurrentWater))
          (Variables|Default|SetCurrentWater Value)
          (Variables|Default|SetCrystal%20size (Variables|Default|GetCurrentCrystal%20size))
          (Variables|Default|SetdesiredCrystal%20size (* (Default|GetSubStats (Variables|Default|GetEquippedStat%20Component) "NewEnumerator37") 0.2))
          (Variables|Default|SetLoc (Variables|Default|GetcurrentLoc))
          (bind _resize (Timeline|IcesizeTime PlayFromStart)
            (:Update
              (bind _output_get (Variables|Default|SetCurrentCrystal%20size (Math|Float|Lerp (Variables|Default|GetCrystal%20size) (Variables|Default|GetdesiredCrystal%20size) _resize)))
              (Niagara|SetNiagaraVariable(Float) (Variables|Default|GetN_FloatingCrystal) "Scale" _output_get)
              (bind _output_get_2 (Variables|Default|SetcurrentLoc (Math|Vector|Lerp(Vector) (Math|Vector|MakeVector 2e+01 0.0 (.z (Variables|Default|GetLoc))) (Math|Vector|MakeVector 2e+01 0.0 (+ (* (* (Default|GetSubStats (Variables|Default|GetEquippedStat%20Component) "NewEnumerator37") 3.0) -1.0) -45.0)) _resize)))
              (Transformation|SetRelativeLocation (Variables|Default|GetItemStaticMesh) _output_get_2 false false)))
          (else
            (Variables|Default|SetCurrentWater Value)
            (bind _output_get_3 (Variables|Default|SetdesiredCrystal%20size (* (Default|GetSubStats (Variables|Default|GetEquippedStat%20Component) "NewEnumerator37") 0.2)))
            (Niagara|SetNiagaraVariable(Float) (Variables|Default|GetN_FloatingCrystal) "Scale" _output_get_3)
            (Transformation|SetRelativeLocation (Variables|Default|GetItemStaticMesh) (Math|Vector|MakeVector 2e+01 0.0 (+ (* (* (Default|GetSubStats (Variables|Default|GetEquippedStat%20Component) "NewEnumerator37") 3.0) -1.0) -45.0)) false false)))))))

(event Custom|RegenWater
  ;[1 1 1] Timer
  (if (not (Utilities|Time|IsValidTimerHandle (Variables|Default|GetTimer)))
    _
    (else
      (Utilities|Time|ClearandInvalidateTimerbyHandle (Variables|Default|GetTimer))))
  (bind _returnvalue (Utilities|Time|SetTimerbyFunctionName 0 "GiveWater" 3.0 true))
  (Variables|Default|SetTimer _returnvalue))

(event Custom|GiveWater
  (bind _visualstatsbuff (Variables|Default|GetVisualStatsBuff))
  (bind _value (Utilities|Map|Find _visualstatsbuff "NewEnumerator8"))
  (bind _returnvalue (/ _value 3.0))
  (bind _returnvalue_2 (* _returnvalue 0.1))
  ;[1 1 1] Timer
  (if (> _returnvalue_2 0.0)
    (Default|ModifyCurrentSubStatValue (Variables|Default|GetEquippedStat%20Component) "NewEnumerator37" _returnvalue_2)
    (Default|ModifySkillXP (Variables|Default|GetEquippedStat%20Component) (.SkillToUse (Utilities|Struct|BreakS_ItemInfo (Variables|Default|GetItemInfo))) (Math|Float|Truncate _returnvalue) true)
    (else
      (Utilities|Time|ClearandInvalidateTimerbyHandle (Variables|Default|GetTimer)))))

(event Custom|CheckTimer
  (bind _equippedstat_component (Variables|Default|GetEquippedStat%20Component))
  ;[1 1 1] Check timer. (stops and sarts timer when needed)
  (if (not (== (Default|GetSubStats _equippedstat_component "NewEnumerator37") (Default|GetMaxSubStats _equippedstat_component "NewEnumerator37")))
    (if (not (Utilities|Time|IsValidTimerHandle (Variables|Default|GetTimer)))
      (CallFunction|RegenWater))
    (else
      (Utilities|Time|ClearandInvalidateTimerbyHandle (Variables|Default|GetTimer)))))

(event EventBeginPlay
  (|CallParentFunction))

(event Collision|EventActorBeginOverlap
  (params (OtherActor :type Actor%20Object%20Reference))
  (|CallParentFunction OtherActor) ; This node is disabled and will not be called.\nDrag off pins to build functionality.
)

(event EventTick
  (params (DeltaSeconds :type Float%20%28single-precision%29))
  (|CallParentFunction DeltaSeconds))

(fn ConstructionScript
  (|CallParentFunction))

(fn RemoveEquipMesh
  (bind _n_floatingcrystal (Variables|Default|GetN_FloatingCrystal))
  (|CallParentFunction)
  (Utilities|IsValid _n_floatingcrystal
    (:Is%20Valid
      (Components|DestroyComponent _n_floatingcrystal))))

(fn RemoveDropMesh
  (bind _n_floatingcrystaldrop (Variables|Default|GetN_FloatingCrystalDrop))
  (|CallParentFunction)
  (Utilities|IsValid _n_floatingcrystaldrop
    (:Is%20Valid
      (Components|DestroyComponent _n_floatingcrystaldrop))))

(fn OnEquipped
  (|CallParentFunction)
  (EventDispatchers|BindEventtoOnMStatsUpdated (Variables|Default|GetEquippedStat%20Component) (EventDispatchers|CreateEvent :!event Custom|Update%20Water))
  (Niagara|SetNiagaraVariable(Float) (Variables|Default|GetN_FloatingCrystal) "Scale" 0.1)
  (CallFunction|RegenWater))

(fn UseAbility
  (bind _inventory (Variables|Default|GetInventory))
  (bind _player (Variables|/Game/DATA/Blueprints/Actors/Inventory/BP_Inventory.BP_Inventory_C|GetPlayer _inventory))
  ;[1 1 1] This is depricated. (now happens in the inventory it's self and GA is set in item info skill struct)
  (bind _returnvalue (Game|SpawnActorfromClass "/Game/DATA/Blueprints/Abilities/GA_PlayerGatherWater.GA_PlayerGatherWater_C" (Math|Transform|MakeTransform "0, 0, 0" "0, 0, 0" "1.000000,1.000000,1.000000") "Undefined" "MultiplyWithRoot" _player (Variables|Default|GetKeyIndex) _player))
  (Class|GamePlayAbilitiesBPI|GAStart(Message) _returnvalue)
  (Actor|DestroyActor))