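; Charged Slash skill actor that temporarily enlarges the player's main weapon hit area, scaled by the skill's Effectiveness.
; Grow swaps weapon collision to its static mesh, widens the capped trace radius, and timeline-scales the mesh and Niagara trail.
; A retriggerable delay in the timeline update calls Shrink seconds after growth ends, restoring collision, reversing the scale and destroying the actor.
; UseAbility is deprecated and empty.
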(event Custom|Grow
  (bind _player (Variables|Default|GetPlayer))
  (bind _player_2 (Variables|Default|GetPlayer))
  (bind _itemstaticmesh (Variables|Default|GetItemStaticMesh))
  (bind _player_3 (Variables|Default|GetPlayer))
  (bind _statscomponent (Variables|/Game/DATA/BP_PC.BP_PC_C|GetStatsComponent _player))
  (bind _combatcomponent (Variables|/Game/DATA/BP_PC.BP_PC_C|GetCombatComponent _player_3))
  (bind _combatcomponent_2 (Variables|/Game/DATA/BP_PC.BP_PC_C|GetCombatComponent _player_2))
  (bind _effectiveness (Default|GetSkillStats _statscomponent "(TagName=\"Character.Action.Skill/Magic.ChargedSlash\")"))
  (bind _returnvalue (Default|GetMainWeapon _combatcomponent))
  (bind _returnvalue_2 (Default|GetMainWeapon _combatcomponent_2))
  (bind _mainweaponcollisioncomponent (Variables|/Game/DATA/Blueprints/Actors/BP_BaseWeapon.BP_BaseWeapon_C|GetMainWeaponCollisionComponent _returnvalue))
  (bind _mainweaponcollisioncomponent_2 (Variables|/Game/DATA/Blueprints/Actors/BP_BaseWeapon.BP_BaseWeapon_C|GetMainWeaponCollisionComponent _returnvalue_2))
  ;[1 1 1] Grow
  (Variables|Default|SetDefault%20Collision%20Capsule%20Component (Variables|/Game/DATA/Blueprints/Components/CollosionComponent.CollosionComponent_C|GetCollisionCapsuleComponent _mainweaponcollisioncomponent))
  (Variables|Default|SetDefault%20Trace%20Radius (Variables|/Game/DATA/Blueprints/Components/CollosionComponent.CollosionComponent_C|GetTraceRadius _mainweaponcollisioncomponent))
  (Default|SetCollisionMesh _mainweaponcollisioncomponent _itemstaticmesh _itemstaticmesh)
  (Variables|/Game/DATA/Blueprints/Components/CollosionComponent.CollosionComponent_C|SetTraceRadius _mainweaponcollisioncomponent_2 (Math|Float|Clamp(Float) (* (* (Variables|/Game/DATA/Blueprints/Components/CollosionComponent.CollosionComponent_C|GetTraceRadius _mainweaponcollisioncomponent_2) 2.0) (.Effectiveness (Default|GetSkillStats (Variables|/Game/DATA/BP_PC.BP_PC_C|GetStatsComponent (Variables|Default|GetPlayer)) "(TagName=\"Character.Action.Skill/Magic.ChargedSlash\")"))) (* (* (Variables|/Game/DATA/Blueprints/Components/CollosionComponent.CollosionComponent_C|GetTraceRadius _mainweaponcollisioncomponent_2) 2.0) (.Effectiveness (Default|GetSkillStats (Variables|/Game/DATA/BP_PC.BP_PC_C|GetStatsComponent (Variables|Default|GetPlayer)) "(TagName=\"Character.Action.Skill/Magic.ChargedSlash\")"))) 75.0))
  (bind _grow (Timeline|Timeline_1 PlayFromStart)
    (:Update
      (Transformation|SetWorldScale3D (Variables|Default|GetItemStaticMesh) (Math|Vector|MakeVector (Math|Float|Clamp(Float) (Math|Float|Lerp 0.0 (* _effectiveness 2.0) _grow) (Math|Float|Lerp 0.0 (* _effectiveness 2.0) _grow) 5.0) (Math|Float|Clamp(Float) (Math|Float|Lerp 0.0 (* _effectiveness 2.0) _grow) (Math|Float|Lerp 0.0 (* _effectiveness 2.0) _grow) 5.0) (Math|Float|Lerp 0.0 (* _effectiveness 2.0) _grow)))
      (Niagara|SetNiagaraVariable(Float) (Variables|Default|GetN_WeaponTrail) "Ribbon Width" (Math|Float|Lerp 0.0 (* _effectiveness 1e+02) _grow))
      (Utilities|FlowControl|RetriggerableDelay 5.0)
      (CallFunction|Shrink))))

(event Custom|Shrink
  (bind _default_collision_capsule_component (Variables|Default|GetDefault%20Collision%20Capsule%20Component))
  ;[1 1 1] Shrink
  (Default|SetCollisionMesh (Variables|/Game/DATA/Blueprints/Actors/BP_BaseWeapon.BP_BaseWeapon_C|GetMainWeaponCollisionComponent (Default|GetMainWeapon (Variables|/Game/DATA/BP_PC.BP_PC_C|GetCombatComponent (Variables|Default|GetPlayer)))) _default_collision_capsule_component _default_collision_capsule_component)
  (Variables|/Game/DATA/Blueprints/Components/CollosionComponent.CollosionComponent_C|SetTraceRadius (Variables|/Game/DATA/Blueprints/Actors/BP_BaseWeapon.BP_BaseWeapon_C|GetMainWeaponCollisionComponent (Default|GetMainWeapon (Variables|/Game/DATA/BP_PC.BP_PC_C|GetCombatComponent (Variables|Default|GetPlayer)))) (Variables|Default|GetDefault%20Trace%20Radius))
  (bind _grow (Timeline|Timeline_2 ReverseFromEnd)
    (:Update
      (Transformation|SetWorldScale3D (Variables|Default|GetItemStaticMesh) (Math|Conversions|ToVector(Float) (Math|Float|Lerp 0.0 (* (.Effectiveness (Default|GetSkillStats (Variables|/Game/DATA/BP_PC.BP_PC_C|GetStatsComponent (Variables|Default|GetPlayer)) "(TagName=\"Character.Action.Skill/Magic.ChargedSlash\")")) 2.0) _grow))))
    (:Finished
      (Actor|DestroyActor))))

(event EventBeginPlay
  (|CallParentFunction) ; This node is disabled and will not be called.\nDrag off pins to build functionality.
)

(event Collision|EventActorBeginOverlap
  (params (OtherActor :type Actor%20Object%20Reference)))

(event EventTick
  (params (DeltaSeconds :type Float%20%28single-precision%29)))

(fn ConstructionScript
  (|CallParentFunction))

(fn UseAbility
  ;[1 1 1] This is depricated. (now happens in the inventory it's self and GA is set in item info skill struct)
)