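; BP_WindpullItem is a useable item actor named for the Wind Pull skill, with no active logic of its own beyond calling its parent construction script.
; UseAbility is an empty, deprecated override, as its comment says the inventory now handles use and the item info skill struct sets the gameplay ability.
; Leftover unconnected nodes would unlock Wind Pull in the skills menu or spawn GA_EnchantWeapon on the player.
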(event EventBeginPlay
  (|CallParentFunction) ; This node is disabled and will not be called.\nDrag off pins to build functionality.
)

(event Collision|EventActorBeginOverlap
  (params (OtherActor :type Actor%20Object%20Reference)))

(event EventTick
  (params (DeltaSeconds :type Float%20%28single-precision%29)))

(fn ConstructionScript
  (|CallParentFunction))

(fn UseAbility
  ;[1 1 1] This is depricated. (now happens in the inventory it's self and GA is set in item info skill struct)
)