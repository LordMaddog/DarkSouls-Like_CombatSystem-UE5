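; BP_GrapplingHookItem is a useable inventory item actor that triggers the player's grappling hook.
; Its UseAbility runs once without calling the parent version, calling GrapplingCast on the player's CombatComponent and then destroying the item.
; The cast value scales from the GrappleHook skill's Power when the StatsComponent uses advanced leveling, and otherwise falls back to a fixed default.
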(event EventBeginPlay
  (|CallParentFunction) ; This node is disabled and will not be called.\nDrag off pins to build functionality.
)

(event Collision|EventActorBeginOverlap
  (params (OtherActor :type Actor%20Object%20Reference)))

(event EventTick
  (params (DeltaSeconds :type Float%20%28single-precision%29)))

(fn ConstructionScript
  (|CallParentFunction))

(fn UseAbility
  (Utilities|FlowControl|DoOnce false
    (:Completed
      (Default|GrapplingCast (Variables|/Game/DATA/BP_PC.BP_PC_C|GetCombatComponent (Variables|/Game/DATA/Blueprints/Actors/Inventory/BP_Inventory.BP_Inventory_C|GetPlayer (Variables|Default|GetInventory))) (select (Variables|/Game/DATA/Blueprints/Components/StatsComponent.StatsComponent_C|GetUseAdvanceLeveling (Variables|/Game/DATA/BP_PC.BP_PC_C|GetStatsComponent (Variables|/Game/DATA/Blueprints/Actors/Inventory/BP_Inventory.BP_Inventory_C|GetPlayer (Variables|Default|GetInventory)))) (* (.Power (Default|GetSkillStats (Variables|/Game/DATA/BP_PC.BP_PC_C|GetStatsComponent (Variables|/Game/DATA/Blueprints/Actors/Inventory/BP_Inventory.BP_Inventory_C|GetPlayer (Variables|Default|GetInventory))) "(TagName=\"Character.Action.Skill/Magic.GrappleHook\")")) 1e+02) 6e+03))
      (Actor|DestroyActor))))