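; BP_RuneStone is an equippable artifact that gives its wearer a chance to retaliate with a knockback spell when damaged.
; On equip, it binds Retaliate to the character's combat component and randomly offsets the NRuneStone component's position.
; Retaliate rolls roughly 40% odds to spawn BP_KnockBackSpell as a stationary area effect on the wearer.
; An unconnected stat-restore branch with a potion burst effect never runs.
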(event Custom|Retaliate
  (bind _equipped_character (Variables|Default|GetEquipped%20Character))
  (if (> (Math|Random|RandomFloatinRange 1.0 1e+02) 6e+01)
    (Game|SpawnActorfromClass :Class "/Game/DATA/Blueprints/Actors/Magic/BP_KnockBackSpell.BP_KnockBackSpell_C" :SpawnTransform (Math|Transform|MakeTransform (Transformation|GetActorLocation (Variables|Default|GetEquipped%20Character)) "0, 0, 0" "1.000000,1.000000,1.000000") :CollisionHandlingOverride "Undefined" :TransformScaleMethod "MultiplyWithRoot" :Owner _equipped_character :AreaEffect 4e+02 :MaxRange 1e+04 :Initial%20Speed 0.0 :Character _equipped_character :Instigator _equipped_character)))

(event Custom|EquippedStart
  (EventDispatchers|BindEventtoReceivedDamage (Variables|/Game/DATA/BP_PC.BP_PC_C|GetCombatComponent (Variables|Default|GetEquipped%20Character)) (delegate Custom|Retaliate)))

(event EventBeginPlay
  (|CallParentFunction))

(event Collision|EventActorBeginOverlap
  (params (OtherActor :type Actor%20Object%20Reference))
  (|CallParentFunction OtherActor) ; This node is disabled and will not be called.\nDrag off pins to build functionality.
)

(event EventTick
  (params (DeltaSeconds :type Float%20%28single-precision%29))
  (|CallParentFunction DeltaSeconds))

(fn ConstructionScript
  (|CallParentFunction))

(fn RemoveEquipMesh
  (bind _n_runestone (Variables|Default|GetN_RuneStone))
  (|CallParentFunction)
  (Utilities|IsValid _n_runestone
    (:Is%20Valid
      (Components|DestroyComponent _n_runestone))))

(fn OnEquipped
  (Variables|Default|SetEquipType (Variables|Default|GetDesiredEquipType))
  (|CallParentFunction)
  (CallFunction|EquippedStart)
  (CallFunction|SetRandomLoc (Variables|Default|GetN_RuneStone)))

(fn SetRandomLoc
  (params (Target :type Scene%20Component%20Object%20Reference))
  (Transformation|SetRelativeLocation Target (Math|Vector|MakeVector (.x (Variables|/Script/Engine.SceneComponent|GetRelativeLocation Target)) (Math|Random|RandomFloatinRange -3e+01 2e+02) (Math|Random|RandomFloatinRange -3e+01 2e+02)) false true))