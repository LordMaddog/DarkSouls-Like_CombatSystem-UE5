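; Magic potion artifact that, once equipped, periodically heals its character by a random amount.
; OnEquipped randomizes the floating Niagara component's relative Y/Z offset and starts RandomHeal, a self-calling loop with a random delay.
; Each pass adds a value capped by a character sub-stat, starts regen, and spawns a burst effect sized to that value.
; Removing the equipped mesh also destroys the floating effect.
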(event Custom|RandomHeal
  (Utilities|FlowControl|Delay (Math|Random|RandomFloatinRange 1.0 3e+01))
  (bind _output_get (Variables|Default|SetRandomValue (Math|Random|RandomFloatinRange 1.0 (Default|GetSubStats (Variables|/Game/DATA/BP_PC.BP_PC_C|GetStatsComponent (Variables|Default|GetEquipped%20Character)) "NewEnumerator12"))))
  (Default|ModifyCurrentStatValue (Variables|/Game/DATA/BP_PC.BP_PC_C|GetStatsComponent (Variables|Default|GetEquipped%20Character)) "NewEnumerator4" _output_get true)
  (bind _returnvalue (Niagara|SpawnSystematLocation "/Game/DATA/Effects/N_MagicPotionBurst.N_MagicPotionBurst" (Transformation|GetActorLocation (Variables|Default|GetEquipped%20Character))))
  (Class|NiagaraComponent|SetVariableInt _returnvalue "SpawnBurst" (Math|Float|Truncate (* (Variables|Default|GetRandomValue) 5.0)))
  (CallFunction|RandomHeal))

(event EventBeginPlay
  (|CallParentFunction))

(event Collision|EventActorBeginOverlap
  (params (OtherActor :type Actor%20Object%20Reference))
  (|CallParentFunction OtherActor) ; This node is disabled and will not be called.\nDrag off pins to build functionality.
)

(event EventTick
  (params (DeltaSeconds :type Float%20%28single-precision%29))
  (|CallParentFunction DeltaSeconds))

(fn ConstructionScript
  (|CallParentFunction))

(fn RemoveEquipMesh
  (bind _n_floatingbible (Variables|Default|GetN_FloatingBible))
  (|CallParentFunction)
  (Utilities|IsValid _n_floatingbible
    (:Is%20Valid
      (Components|DestroyComponent _n_floatingbible))))

(fn OnEquipped
  (Variables|Default|SetEquipType (Variables|Default|GetDesiredEquipType))
  (|CallParentFunction)
  (CallFunction|SetRandomLoc (Variables|Default|GetN_FloatingBible))
  (CallFunction|RandomHeal))

(fn SetRandomLoc
  (params (Target :type Scene%20Component%20Object%20Reference))
  (Transformation|SetRelativeLocation Target (Math|Vector|MakeVector (.x (Variables|/Script/Engine.SceneComponent|GetRelativeLocation Target)) (Math|Random|RandomFloatinRange -3e+01 2e+02) (Math|Random|RandomFloatinRange -3e+01 2e+02)) false true))