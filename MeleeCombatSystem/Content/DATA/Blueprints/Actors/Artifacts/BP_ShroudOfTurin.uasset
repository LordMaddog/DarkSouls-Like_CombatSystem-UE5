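; Shroud of Turin artifact that saves its equipped character from one death, then recharges after the character resurrects.
; On equip it blocks death and binds to the would-have-died and resurrect events, placing its mesh at a randomized offset.
; A would-be death fires once, toggling off flight, breaking poise, spawning a full heal spell, then re-enabling death and hiding the mesh.
; Resurrection re-arms it after a delay; unequipping restores mortality.
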(event Custom|Ressurect
  (bind _equipped_character (Variables|Default|GetEquipped%20Character))
  (bind _equipped_character_2 (Variables|Default|GetEquipped%20Character))
  (bind _equipped_character_3 (Variables|Default|GetEquipped%20Character))
  (bind _combatcomponent (Variables|/Game/DATA/BP_PC.BP_PC_C|GetCombatComponent _equipped_character))
  (Utilities|FlowControl|DoOnce false
    (:Completed
      (if (not (Variables|/Game/DATA/Blueprints/Components/CombatComponent.CombatComponent_C|GetbFlying _combatcomponent))
        _
        (else
          (Default|Fly _combatcomponent)
          (Utilities|FlowControl|Delay 0.2)))
      (Default|PoiseBreak (Variables|Default|GetEquipped%20Character))
      (Utilities|FlowControl|Delay 1.0)
      (bind _returnvalue (Game|SpawnActorfromClass :Class "/Game/DATA/Blueprints/Actors/Magic/BP_HealShieldSpell.BP_HealShieldSpell_C" :SpawnTransform (Math|Transform|MakeTransform (Transformation|GetActorLocation _equipped_character_3) (Transformation|GetActorRotation _equipped_character_3) "1.000000,1.000000,1.000000") :CollisionHandlingOverride "Undefined" :TransformScaleMethod "MultiplyWithRoot" :Owner _equipped_character_2 :MaxRange 1e+04 :Initial%20Speed 0.0 :Character _equipped_character_2 :FriendlyFire? true :HealSpell true :Instigator _equipped_character_2))
      (Variables|/Game/DATA/Blueprints/Actors/BP_BaseSpell.BP_BaseSpell_C|SetHealPower _returnvalue (* (Default|GetMaxStatValue (Variables|/Game/DATA/BP_PC.BP_PC_C|GetStatsComponent (Variables|Default|GetEquipped%20Character)) "NewEnumerator1") -1.0))
      (Variables|/Game/DATA/Blueprints/Components/StatsComponent.StatsComponent_C|SetCanDie (Variables|/Game/DATA/BP_PC.BP_PC_C|GetStatsComponent (Variables|Default|GetEquipped%20Character)) true)
      (Rendering|SetVisibility (Variables|Default|GetN_ShroudOfTurin) false false))))

(event Custom|EquippedStart
  (bind _equipped_character (Variables|Default|GetEquipped%20Character))
  (Variables|/Game/DATA/Blueprints/Components/StatsComponent.StatsComponent_C|SetCanDie (Variables|/Game/DATA/BP_PC.BP_PC_C|GetStatsComponent (Variables|Default|GetEquipped%20Character)) false)
  (EventDispatchers|BindEventtoWouldHaveDied (Variables|/Game/DATA/BP_PC.BP_PC_C|GetStatsComponent _equipped_character) (delegate Custom|Ressurect))
  (EventDispatchers|BindEventtoResurrectDispatch (Variables|/Game/DATA/BP_PC.BP_PC_C|GetCombatComponent _equipped_character) (delegate Custom|DieAndReset)))

(event Custom|DieAndReset
  (Utilities|FlowControl|Delay 3.0)
  (Variables|/Game/DATA/Blueprints/Components/StatsComponent.StatsComponent_C|SetCanDie (Variables|/Game/DATA/BP_PC.BP_PC_C|GetStatsComponent (Variables|Default|GetEquipped%20Character)) false)
  (Rendering|SetVisibility (Variables|Default|GetN_ShroudOfTurin) true false)
  (CallFunction|Reset))

(event Custom|Reset
  (bind _equipped_character (Variables|Default|GetEquipped%20Character))
  (bind _equipped_character_2 (Variables|Default|GetEquipped%20Character))
  (bind _equipped_character_3 (Variables|Default|GetEquipped%20Character))
  (bind _combatcomponent (Variables|/Game/DATA/BP_PC.BP_PC_C|GetCombatComponent _equipped_character))
  (Utilities|FlowControl|DoOnce false) ; enters at Reset
)

(event EventBeginPlay
  (|CallParentFunction))

(event Collision|EventActorBeginOverlap
  (params (OtherActor :type Actor%20Object%20Reference))
  (|CallParentFunction OtherActor) ; This node is disabled and will not be called.\nDrag off pins to build functionality.
)

(event EventTick
  (params (DeltaSeconds :type Float%20%28single-precision%29))
  (|CallParentFunction DeltaSeconds))

(fn ConstructionScript
  (|CallParentFunction))

(fn RemoveEquipMesh
  (bind _n_shroudofturin (Variables|Default|GetN_ShroudOfTurin))
  (|CallParentFunction)
  (Utilities|IsValid _n_shroudofturin
    (:Is%20Valid
      (Components|DestroyComponent _n_shroudofturin))))

(fn OnEquipped
  (Variables|Default|SetEquipType (Variables|Default|GetDesiredEquipType))
  (|CallParentFunction)
  (CallFunction|SetRandomLoc (Variables|Default|GetN_ShroudOfTurin))
  (CallFunction|EquippedStart))

(fn SetRandomLoc
  (params (Target :type Scene%20Component%20Object%20Reference))
  (Transformation|SetRelativeLocation Target (Math|Vector|MakeVector (Math|Random|RandomFloatinRange 1.3e+02 2e+02) (.y (Variables|/Script/Engine.SceneComponent|GetRelativeLocation Target)) (Math|Random|RandomFloatinRange -3e+01 2e+02)) false true))

(fn OnUnequipped
  (params (GiveBack? :type Boolean) (ForceDrop :type Boolean) (ItemInfoIn :type S%20Item%20Info%20Structure))
  (|CallParentFunction GiveBack? ForceDrop ItemInfoIn)
  (Variables|/Game/DATA/Blueprints/Components/StatsComponent.StatsComponent_C|SetCanDie (Variables|/Game/DATA/BP_PC.BP_PC_C|GetStatsComponent (Variables|Default|GetEquipped%20Character)) true))