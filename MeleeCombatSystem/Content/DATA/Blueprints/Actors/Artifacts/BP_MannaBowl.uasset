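; Mana bowl artifact that, while equipped, periodically flies off its wearer to cast an area heal spell nearby.
; After a random delay, RandomHeal traces toward a random reachable point, with a second trace toward a fixed low point on a miss.
; A timeline flies the detached bowl to the hit, spawns BP_MannaBowlSpell and hides the bowl on it.
; ArtifactSpellDone reattaches the bowl, flies it back and restarts the cycle.
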(event Custom|RandomHeal
  (bind _equipped_character (Variables|Default|GetEquipped%20Character))
  (bind _equipped_character_2 (Variables|Default|GetEquipped%20Character))
  (bind _returnvalue (Transformation|GetActorLocation _equipped_character_2))
  (bind _returnvalue_2 (+ _returnvalue "0.000000,0.000000,50.000000"))
  (Utilities|FlowControl|Sequence
    (:then_0
      (Utilities|FlowControl|Delay (Math|Random|RandomFloatinRange 1.0 2e+01))
      (bind _outhit (Collision|LineTraceByChannel _returnvalue_2 (.RandomLocation (AI|Navigation|GetRandomReachablePointinRadius _returnvalue_2 1.5e+03 0 0)) "TraceTypeQuery1" false (Utilities|Array|MakeArray (Variables|Default|GetEquipped%20Character)) "None"))
      (if (.bBlockingHit (Collision|BreakHitResult _outhit))
        (Variables|Default|SetSpawnLoc (select (.bBlockingHit (Collision|BreakHitResult _outhit)) (.Location (Collision|BreakHitResult _outhit)) (.Location (Collision|BreakHitResult (stale _outhit_2)))) :!label _label)
        (Variables|Default|SetCurrentLocation (Transformation|GetWorldLocation (Variables|Default|GetN_MannaBowl)))
        (Transformation|DetachFromComponent (Variables|Default|GetN_MannaBowl) "KeepWorld" "KeepWorld" "KeepWorld" true)
        (bind _fly (Timeline|Timeline_1 PlayFromStart)
          (:Update
            (Transformation|SetWorldLocation (Variables|Default|GetN_MannaBowl) (Math|Vector|Lerp(Vector) (Variables|Default|GetCurrentLocation) (Variables|Default|GetSpawnLoc) _fly) false true))
          (:Finished
            (Utilities|FlowControl|Delay 0.5)
            (bind _returnvalue_3 (Game|SpawnActorfromClass :Class "/Game/DATA/Blueprints/Actors/Magic/BP_MannaBowlSpell.BP_MannaBowlSpell_C" :SpawnTransform (Math|Transform|MakeTransform (Variables|Default|GetSpawnLoc) (Math|Rotator|MakeRotator (.roll (Math|Rotator|FindLookatRotation (Variables|Default|GetSpawnLoc) (Transformation|GetActorLocation (Variables|Default|GetEquipped%20Character)))) 0.0 0.0) "1.000000,1.000000,1.000000") :CollisionHandlingOverride "Undefined" :TransformScaleMethod "MultiplyWithRoot" :Owner _equipped_character :Spawner self :AreaEffect 45.0 :MaxRange 4e+03 :Initial%20Speed 0.0 :Character _equipped_character :FriendlyFire? true :HealSpell true :HealPower -1e+01 :Instigator _equipped_character))
            (Transformation|AttachComponentToComponent (Variables|Default|GetN_MannaBowl) (Variables|/Game/DATA/Blueprints/Actors/Magic/BP_MannaBowlSpell.BP_MannaBowlSpell_C|GetMannaBowl _returnvalue_3) "None" "KeepWorld" "KeepWorld" "KeepWorld" true)
            (Rendering|SetVisibility (Variables|Default|GetN_MannaBowl) false false)
            (Transformation|SetWorldRotation (Variables|Default|GetN_MannaBowl) "0, 0, 0" false false)
            (Transformation|SetRelativeLocation (Variables|Default|GetN_MannaBowl) (Variables|Default|GetDefault%20Relative%20Location) false true)))
        (else
          (bind _outhit_2 (Collision|LineTraceByChannel (.TraceEnd (Collision|BreakHitResult _outhit)) "0.000000,0.000000,-1000.000000" "TraceTypeQuery1" false 0 "None"))
          (if (.bBlockingHit (Collision|BreakHitResult _outhit_2))
            (goto _label)))))
    (:then_1
      (Utilities|FlowControl|DoOnce false
        (:Completed
          (Variables|Default|SetDefault%20Relative%20Location (Variables|/Script/Engine.SceneComponent|GetRelativeLocation (Variables|Default|GetN_MannaBowl))))))))

(event EventBeginPlay
  (|CallParentFunction))

(event Collision|EventActorBeginOverlap
  (params (OtherActor :type Actor%20Object%20Reference))
  (|CallParentFunction OtherActor) ; This node is disabled and will not be called.\nDrag off pins to build functionality.
)

(event EventTick
  (params (DeltaSeconds :type Float%20%28single-precision%29))
  (|CallParentFunction DeltaSeconds))

(event EventArtifactSpellDone
  (params (Index :type Integer))
  (CallFunction|RandomHeal)
  (Rendering|SetVisibility (Variables|Default|GetN_MannaBowl) true false)
  (Transformation|AttachComponentToComponent (Variables|Default|GetN_MannaBowl) (Variables|Default|GetItemStaticMesh) "None" "KeepWorld" "KeepWorld" "KeepWorld" true)
  (Transformation|SetWorldRotation (Variables|Default|GetN_MannaBowl) "0, 0, 0" false false)
  (Variables|Default|SetCurrentLocation (Variables|/Script/Engine.SceneComponent|GetRelativeLocation (Variables|Default|GetN_MannaBowl)))
  (bind _fly (Timeline|Fly%20Back PlayFromStart)
    (:Update
      (Transformation|SetRelativeLocation (Variables|Default|GetN_MannaBowl) (Math|Vector|Lerp(Vector) (Variables|Default|GetCurrentLocation) (Variables|Default|GetDefault%20Relative%20Location) _fly) false true))))

(fn ConstructionScript
  (|CallParentFunction))

(fn RemoveEquipMesh
  (bind _n_mannabowl (Variables|Default|GetN_MannaBowl))
  (|CallParentFunction)
  (Utilities|IsValid _n_mannabowl
    (:Is%20Valid
      (Components|DestroyComponent _n_mannabowl))))

(fn OnEquipped
  (Variables|Default|SetEquipType (Variables|Default|GetDesiredEquipType))
  (|CallParentFunction)
  (CallFunction|SetRandomLoc (Variables|Default|GetN_MannaBowl))
  (CallFunction|RandomHeal))

(fn SetRandomLoc
  (params (Target :type Scene%20Component%20Object%20Reference))
  (Transformation|SetRelativeLocation Target (Math|Vector|MakeVector (.x (Variables|/Script/Engine.SceneComponent|GetRelativeLocation Target)) (Math|Random|RandomFloatinRange -3e+01 2e+02) (Math|Random|RandomFloatinRange -3e+01 2e+02)) false true))

(fn CanReciveDamage
  (return false))

(fn CheckifCanbeBackstabbed
  (params (HitLoc :type Vector :default "0, 0, 0") (Attacker :type BP%20PC%20Object%20Reference))
  (return false ""))

(fn DamageType
  (return "NewEnumerator0"))

(fn GetCharacterInfo
  (return 0))

(fn GetDesiredRotation
  (return "0, 0, 0"))

(fn PreformCombatAction
  (params (ActionTag :type Gameplay%20Tag%20Structure) (SateTag :type Gameplay%20Tag%20Structure) (MontageIndex :type Integer) (bRandomItemIndex :type Boolean))
  (return 0.0))

(fn PreformCombatAttack
  (params (AttackType :type Gameplay%20Tag%20Structure) (SetState :type Gameplay%20Tag%20Structure) (AttackIndex :type Integer) (bRandomIndex :type Boolean) (WeaponBased :type Boolean))
  (return 0.0))

(fn PreformCustomAction
  (params (ActionTag :type Gameplay%20Tag%20Structure) (StateTag :type Gameplay%20Tag%20Structure) (InMontage :type Anim%20Montage%20Object%20Reference) (MontagePlayRate :type Float%20%28double-precision%29) (bAutoReset :type Boolean))
  (return false))

(fn UpdateMotionWarp
  (params (Name :type Name :default "None") (LOC :type Transform))
  (return "0, 0, 0"))