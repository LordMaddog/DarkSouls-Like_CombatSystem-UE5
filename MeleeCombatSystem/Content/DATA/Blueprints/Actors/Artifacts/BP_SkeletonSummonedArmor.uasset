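; Artifact actor for the skeleton summoned armor, an equippable item that shows a floating bible component while equipped.
; On equip it sets its equip type to the desired type, runs the parent logic, then offsets the bible to a random local Y/Z position, keeping X.
; Removing the equip mesh also destroys the bible component, and all other behavior comes from the parent class.
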(event EventBeginPlay
  (|CallParentFunction))

(event Collision|EventActorBeginOverlap
  (params (OtherActor :type Actor%20Object%20Reference))
  (|CallParentFunction OtherActor) ; This node is disabled and will not be called.\nDrag off pins to build functionality.
)

(event EventTick
  (params (DeltaSeconds :type Float%20%28single-precision%29))
  (|CallParentFunction DeltaSeconds))

(fn ConstructionScript
  (|CallParentFunction))

(fn RemoveEquipMesh
  (bind _n_floatingbible (Variables|Default|GetN_FloatingBible))
  (|CallParentFunction)
  (Utilities|IsValid _n_floatingbible
    (:Is%20Valid
      (Components|DestroyComponent _n_floatingbible))))

(fn SetRandomLoc
  (params (Target :type Scene%20Component%20Object%20Reference))
  (Transformation|SetRelativeLocation Target (Math|Vector|MakeVector (.x (Variables|/Script/Engine.SceneComponent|GetRelativeLocation Target)) (Math|Random|RandomFloatinRange -2e+01 6e+01) (Math|Random|RandomFloatinRange -2e+01 6e+01)) false true))

(fn OnEquipped
  (Variables|Default|SetEquipType (Variables|Default|GetDesiredEquipType))
  (|CallParentFunction)
  (CallFunction|SetRandomLoc (Variables|Default|GetN_FloatingBible)))