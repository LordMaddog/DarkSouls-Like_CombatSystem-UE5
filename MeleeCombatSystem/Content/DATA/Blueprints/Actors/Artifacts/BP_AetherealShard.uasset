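; BP_AetherealShard is an equippable artifact that gives its wearer a chance to heal when taking damage.
; On equip it binds Heal to the CombatComponent's received-damage event and randomly offsets its mesh.
; Heal occasionally spawns BP_HealSpell on the wearer, with a negated random HealPower capped by one of two randomly picked substats.
; An older direct stat-restore with a Niagara burst remains unconnected.
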(event Custom|Heal
  (bind _equipped_character (Variables|Default|GetEquipped%20Character))
  (bind _equipped_character_2 (Variables|Default|GetEquipped%20Character))
  (bind _equipped_character_3 (Variables|Default|GetEquipped%20Character))
  (bind _statscomponent (Variables|/Game/DATA/BP_PC.BP_PC_C|GetStatsComponent _equipped_character_3))
  (if (> (Math|Random|RandomFloatinRange 1.0 1e+02) 8e+01)
    (bind _returnvalue (Game|SpawnActorfromClass :Class "/Game/DATA/Blueprints/Actors/Magic/BP_HealSpell.BP_HealSpell_C" :SpawnTransform (Math|Transform|MakeTransform (Transformation|GetActorLocation _equipped_character_2) (Transformation|GetActorRotation _equipped_character_2) "1.000000,1.000000,1.000000") :CollisionHandlingOverride "Undefined" :TransformScaleMethod "MultiplyWithRoot" :Owner _equipped_character :Character _equipped_character :Instigator _equipped_character))
    (Variables|/Game/DATA/Blueprints/Actors/BP_BaseSpell.BP_BaseSpell_C|SetHealPower _returnvalue (* (Math|Random|RandomFloatinRange 1.0 (select (> (Math|Random|RandomFloatinRange 1.0 1e+02) 5e+01) (Default|GetSubStats _statscomponent "NewEnumerator11") (Default|GetSubStats _statscomponent "NewEnumerator12"))) -1.0))))

(event Custom|EquippedStart
  (EventDispatchers|BindEventtoReceivedDamage (Variables|/Game/DATA/BP_PC.BP_PC_C|GetCombatComponent (Variables|Default|GetEquipped%20Character)) (delegate Custom|Heal)))

(event EventBeginPlay
  (|CallParentFunction))

(event Collision|EventActorBeginOverlap
  (params (OtherActor :type Actor%20Object%20Reference))
  (|CallParentFunction OtherActor) ; This node is disabled and will not be called.\nDrag off pins to build functionality.
)

(event EventTick
  (params (DeltaSeconds :type Float%20%28single-precision%29))
  (|CallParentFunction DeltaSeconds))

(fn ConstructionScript
  (|CallParentFunction))

(fn RemoveEquipMesh
  (bind _n_floatingbible (Variables|Default|GetN_FloatingBible))
  (|CallParentFunction)
  (Utilities|IsValid _n_floatingbible
    (:Is%20Valid
      (Components|DestroyComponent _n_floatingbible))))

(fn OnEquipped
  (Variables|Default|SetEquipType (Variables|Default|GetDesiredEquipType))
  (|CallParentFunction)
  (CallFunction|EquippedStart)
  (CallFunction|SetRandomLoc (Variables|Default|GetItemStaticMesh)))

(fn SetRandomLoc
  (params (Target :type Scene%20Component%20Object%20Reference))
  (Transformation|SetRelativeLocation Target (Math|Vector|MakeVector (.x (Variables|/Script/Engine.SceneComponent|GetRelativeLocation Target)) (Math|Random|RandomFloatinRange -3e+01 1e+02) (Math|Random|RandomFloatinRange -3e+01 1e+02)) false true))