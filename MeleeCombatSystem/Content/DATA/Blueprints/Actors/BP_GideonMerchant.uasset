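; Gideon merchant NPC that shows a "Merchant" label while overlapped and opens a shop on interaction.
; Interact creates a centered shop widget linked to the player's inventory, refreshes that inventory and multiplies its cost multiplier by the merchant discount.
; A DoOnce blocks duplicate shops until OnShopClose removes the widget, without restoring the multiplier.
; ToCastOrNotToCast caches the player BP_PC, then returns true for any actor.
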(event OnComponentBeginOverlap(Box)
  (params (OverlappedComponent :type Primitive%20Component%20Object%20Reference) (OtherActor :type Actor%20Object%20Reference) (OtherComp :type Primitive%20Component%20Object%20Reference) (OtherBodyIndex :type Integer) (bFromSweep :type Boolean) (SweepResult :type Hit%20Result%20Structure%20%28by%20ref%29))
  ;[1 1 1] Add text over Merchants head
  (bind _isplayer (CallFunction|ToCastorNottoCast OtherActor))
  (if _isplayer
    (Rendering|SetVisibility (Variables|Default|GetPickUpText) true false)))

(event OnComponentEndOverlap(Box)
  (params (OverlappedComponent :type Primitive%20Component%20Object%20Reference) (OtherActor :type Actor%20Object%20Reference) (OtherComp :type Primitive%20Component%20Object%20Reference) (OtherBodyIndex :type Integer))
  ;[1 1 1] Add text over Merchants head
  (bind _isplayer (CallFunction|ToCastorNottoCast OtherActor))
  (if _isplayer
    (Rendering|SetVisibility (Variables|Default|GetPickUpText) false false)))

(event Custom|OnShopClose
  (bind _player (Variables|Default|GetPlayer))
  (bind _player_2 (Variables|Default|GetPlayer))
  (bind _player_3 (Variables|Default|GetPlayer))
  (bind _player_4 (Variables|Default|GetPlayer))
  (bind _inventory (Variables|/Game/DATA/BP_PC.BP_PC_C|GetInventory _player))
  (bind _inventory_2 (Variables|/Game/DATA/BP_PC.BP_PC_C|GetInventory _player_2))
  (bind _inventory_3 (Variables|/Game/DATA/BP_PC.BP_PC_C|GetInventory _player_3))
  ;[1 1 1] Open and close Shop Window
  (Variables|/Game/DATA/Blueprints/Actors/Inventory/BP_Inventory.BP_Inventory_C|SetshopOpen (Variables|/Game/DATA/BP_PC.BP_PC_C|GetInventory (Variables|Default|GetPlayer)) false)
  (if (Variables|/Game/DATA/Blueprints/Actors/Inventory/BP_Inventory.BP_Inventory_C|GetInventoryVisible (Variables|/Game/DATA/BP_PC.BP_PC_C|GetInventory (Variables|Default|GetPlayer)))
    (Default|HideInventory _inventory_3)
    (Default|ShowInventory _inventory_3))
  (Widget|RemovefromParent (Variables|Default|GetShopWidget))
  (Variables|Default|SetShopWidget 0)
  (Variables|/Game/DATA/Blueprints/Actors/Inventory/BP_Inventory.BP_Inventory_C|SetShopWidget (Variables|/Game/DATA/BP_PC.BP_PC_C|GetInventory (Variables|Default|GetPlayer)) 0)
  (Utilities|FlowControl|DoOnce false) ; enters at Reset
)

(event EventBeginPlay
  ;[1 1 1] Change text over merchant's head
  (bind _ascw_interact_text (Utilities|Casting|CastToCW_InteractText (UserInterface|GetUserWidgetObject (Variables|Default|GetPickUpText))))
  (Rendering|Components|TextRender|SetText (Variables|/Game/DATA/UI/Inventory/CW_InteractText.CW_InteractText_C|GetNameText _ascw_interact_text) "Merchant")
  (Appearance|SetColorandOpacity (Variables|/Game/DATA/UI/Inventory/CW_InteractText.CW_InteractText_C|GetNameText _ascw_interact_text) (Utilities|Struct|MakeSlateColor "(R=0.405093,G=0.375518,B=0.000000,A=1.000000)") :!class /Script/UMG.TextBlock))

(event EventInteract
  (params (CallEvent :type Actor%20Object%20Reference))
  (bind _player (Variables|Default|GetPlayer))
  (bind _player_2 (Variables|Default|GetPlayer))
  (bind _player_3 (Variables|Default|GetPlayer))
  (bind _inventory (Variables|/Game/DATA/BP_PC.BP_PC_C|GetInventory _player))
  (bind _inventory_2 (Variables|/Game/DATA/BP_PC.BP_PC_C|GetInventory _player_2))
  ;[1 1 1] Open and close Shop Window
  (CallFunction|ToCastorNottoCast CallEvent)
  (Utilities|FlowControl|DoOnce false
    (:Completed
      (bind _returnvalue (UserInterface|CreateWidget "/Game/DATA/UI/Inventory/CW_ShopWidget.CW_ShopWidget_C" 0 self _player_3 (Variables|/Game/DATA/BP_PC.BP_PC_C|GetInventory _player_3)))
      (bind _output_get (Variables|Default|SetShopWidget _returnvalue))
      (Variables|/Game/DATA/Blueprints/Actors/Inventory/BP_Inventory.BP_Inventory_C|SetShopWidget (Variables|/Game/DATA/BP_PC.BP_PC_C|GetInventory (Variables|Default|GetPlayer)) _output_get)
      (Variables|/Game/DATA/Blueprints/Actors/Inventory/BP_Inventory.BP_Inventory_C|SetshopOpen (Variables|/Game/DATA/BP_PC.BP_PC_C|GetInventory (Variables|Default|GetPlayer)) true)
      (Variables|/Game/DATA/Blueprints/Actors/Inventory/BP_Inventory.BP_Inventory_C|SetCostMultiplyer _inventory (* (Variables|Default|GetMerchantDiscount) (Variables|/Game/DATA/Blueprints/Actors/Inventory/BP_Inventory.BP_Inventory_C|GetCostMultiplyer _inventory)))
      (Class|UserWidget|SetPositioninViewport :self (Variables|Default|GetShopWidget) :bRemoveDPIScale false)
      (Class|UserWidget|SetAnchorsinViewport (Variables|Default|GetShopWidget) (Utilities|Struct|MakeAnchors "(X=0.500000,Y=0.500000)" "(X=0.500000,Y=0.500000)"))
      (Class|UserWidget|SetAlignmentinViewport (Variables|Default|GetShopWidget) "(X=0.500000,Y=0.500000)")
      (UserInterface|Viewport|AddtoViewport (Variables|Default|GetShopWidget) 5)
      (Default|HideInventory _inventory_2)
      (Default|ShowInventory _inventory_2))))

(fn ConstructionScript)

(fn ToCastorNottoCast
  (params (InActor :type Actor%20Object%20Reference))
  (bind _player (Variables|Default|GetPlayer)
    (:then
      (if (== (Variables|Default|GetPlayer) _player)
        (return true)))
    (:else
      (bind _asbp_pc (Utilities|Casting|CastToBP_PC InActor)
        (:then
          (if (Variables|/Game/DATA/Blueprints/Components/CombatComponent.CombatComponent_C|GetIsPlayer (Variables|/Game/DATA/BP_PC.BP_PC_C|GetCombatComponent _asbp_pc))
            (Variables|Default|SetPlayer _asbp_pc)
            (return true)))
        (:CastFailed
          (return false))))))