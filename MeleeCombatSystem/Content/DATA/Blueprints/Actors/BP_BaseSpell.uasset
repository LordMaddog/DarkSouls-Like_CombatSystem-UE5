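; Base projectile spell actor that ignores its instigator, records impact info for an empty Hit event, and destroys itself beyond max range.
; Construction sets area radius, initial speed and damage scaled from a caster sub-stat.
; ApplyDamage deals point damage if the target's CombatComponent allows it and, without friendly fire, shares no gameplay tags with the caster.
; Helpers spawn impact decals and compute the poise damage multiplier.
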(event OnComponentHit(MainProjectileCore)
  (params (HitComponent :type Primitive%20Component%20Object%20Reference) (OtherActor :type Actor%20Object%20Reference) (OtherComp :type Primitive%20Component%20Object%20Reference) (NormalImpulse :type Vector :default "0, 0, 0") (Hit :type Hit%20Result%20Structure%20%28by%20ref%29))
  (Variables|Default|SetHitInfo Hit)
  (Variables|Default|SetHitActor OtherActor)
  (CallFunction|Hit))

(event Custom|Hit)

(event EventBeginPlay
  (Collision|IgnoreActorwhenMoving (Variables|/Script/Engine.MovementComponent|GetUpdatedPrimitive (Variables|Default|GetProjectileMovement)) (Game|GetInstigator) true)
  (bind _output_get (Variables|Default|SetStaringPostion (Transformation|GetActorLocation))))

(event EventTick
  (params (DeltaSeconds :type Float%20%28single-precision%29))
  (if (> (Math|Vector|Distance(Vector) (stale EventBeginPlay _output_get) (Transformation|GetActorLocation)) (Variables|Default|GetMaxRange))
    (Utilities|FlowControl|DoOnce false
      (:Completed
        (Actor|DestroyActor)))))

(fn ConstructionScript
  (Components|Sphere|SetSphereRadius (Variables|Default|GetAreaOfEffect) (Variables|Default|GetAreaEffect) true)
  (Variables|/Script/Engine.ProjectileMovementComponent|SetInitialSpeed (Variables|Default|GetProjectileMovement) (Variables|Default|GetInitial%20Speed))
  (CallFunction|DamageCalculate))

(fn DamageCalculate
  (Variables|Default|SetDamageOut (* (Variables|Default|GetDamageMultiplier) (Default|GetSubStats (Variables|/Game/DATA/BP_PC.BP_PC_C|GetStatsComponent (Variables|Default|GetCharacter)) "NewEnumerator12"))))

(fn SpawnDecal
  (params (HitInfo :type Hit%20Result%20Structure) (Decal :type Actor%20Class%20Reference) (ImpactScale :type Float%20%28double-precision%29) (ScaleMatch? :type Boolean) (MatchedScale :type Vector))
  (bind _instigator (Variables|Actor|GetInstigator))
  (Game|SpawnActorfromClass "/Game/DATA/Blueprints/Actors/Utility/BP_DecalSpawnFunction.BP_DecalSpawnFunction_C" (Transformation|GetActorTransform) "Undefined" "MultiplyWithRoot" _instigator HitInfo Decal ImpactScale ScaleMatch? MatchedScale _instigator))

(fn ApplyDamage
  (params (DamagedActor :type Actor%20Object%20Reference) (HitInfo :type Hit%20Result%20Structure%20%28by%20ref%29))
  (bind _damagable_ (CallFunction|TakeDamage? DamagedActor))
  (if _damagable_
    (Game|Damage|ApplyPointDamage DamagedActor (Variables|Default|GetDamageOut) (Transformation|GetWorldLocation (Variables|Default|GetMainProjectileCore)) HitInfo (Game|GetInstigatorController) self (Variables|Default|GetDamage%20Type%20Class))))

(fn TakeDamage?
  (params (DamagedActor :type Actor%20Object%20Reference))
  (if (not (Variables|Default|GetFriendlyFire?))
    (bind _gameplaytags (Class|GameplayTagBPI|GetOwnedGamplayTags(Message) DamagedActor))
    (if (not (GameplayTags|HasAnyTags _gameplaytags (Variables|/Game/DATA/BP_PC.BP_PC_C|GetOwnedGamePlayTags (Variables|Default|GetCharacter)) true))
      _
      (else
        (return false))))
  (bind _returnvalue (Class|CombatBPI|CanReciveDamage(Message) (Actor|GetComponentbyClass DamagedActor "/Game/DATA/Blueprints/Components/CombatComponent.CombatComponent_C")))
  (return _returnvalue))

(fn GetOwnedGamplayTags
  (return ""))

(fn GetPoiseDamageMutltiplier
  (return (* (Variables|Default|GetBasePoiseDamgeMultiplier) (Variables|Default|GetPoiseDamgeMultiplier))))

(fn HasMatchingGamplayTag
  (params (TagsToCheck :type Gameplay%20Tag%20Container%20Structure))
  (return false))