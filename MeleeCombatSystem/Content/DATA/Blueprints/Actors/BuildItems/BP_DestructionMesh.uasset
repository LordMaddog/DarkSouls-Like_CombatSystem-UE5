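; BP_DestructionMesh is a temporary actor that shows a build item breaking apart as a Chaos geometry collection.
; On BeginPlay it assigns the supplied collection, waits a tick-length delay, reveals it, enables physics and fires a radial impulse to scatter the pieces.
; The actor destroys itself when the collection raises a Chaos removal event.
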(event OnChaosRemovalEvent(GeometryCollection)
  (params (RemovalEvent :type Chaos%20Removal%20Event%20Structure%20%28by%20ref%29))
  (Actor|DestroyActor))

(event EventBeginPlay
  (bind _geometrycollection (Variables|Default|GetGeometryCollection))
  (bind _collection_in (Variables|Default|GetCollection%20In)
    (:then
      (Class|GeometryCollectionComponent|SetRestCollection (Variables|Default|GetGeometryCollection) _collection_in)
      (Utilities|FlowControl|Delay 0.01)
      (Development|SetHiddeninGame (Variables|Default|GetGeometryCollection) false false)
      (Rendering|SetVisibility _geometrycollection true false)
      (Physics|SetSimulatePhysics _geometrycollection true)
      (Class|RadialForceComponent|FireImpulse (Variables|Default|GetRadialForce)))
    (:else)))

(fn ConstructionScript)