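; Temporary build-effect actor that animates a part being added to a build actor, then destroys itself.
; On BeginPlay it copies the target component's mesh, applies materials from a lookup and plays briefly audible sound.
; A timeline lerps the copy from zero scale below the target to its transform, feeding bounds to Niagara.
; When finished, it activates the real part through InBuildActor.
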(event Custom|DynamiclyAdd
  (bind _staticmesh (Variables|Default|GetStaticMesh))
  (bind _niagara (Variables|Default|GetNiagara))
  (bind (_origin _boxextent) (Collision|GetComponentBounds _staticmesh))
  (Rendering|SetVisibility (Variables|Default|GetStaticMesh) true false)
  (bind _float (Timeline|FloatTO PlayFromStart)
    (:Update
      (Utilities|IsValid (Variables|Default|GetInStatic%20Mesh)
        (:Is%20Valid
          (Utilities|IsValid (Variables|Default|GetStaticMesh)
            (:Is%20Valid
              (Transformation|SetWorldTransform (Variables|Default|GetStaticMesh) (Math|Transform|Lerp(Transform) (Math|Transform|MakeTransform (+ (Transformation|GetWorldLocation (Variables|Default|GetInStatic%20Mesh)) "0.000000,0.000000,-500.000000") (Transformation|GetWorldRotation (Variables|Default|GetInStatic%20Mesh)) "0.000000,0.000000,0.000000") (Transformation|GetWorldTransform (Variables|Default|GetInStatic%20Mesh)) _float) false false)
              (Effects|Components|ParticleSystem|SetVectorParameter _niagara "BoxExtent" (* _boxextent 2.0))
              (Class|NiagaraComponent|SetVariablePosition _niagara "BoxOrigin" _origin))))
        (:Is%20Not%20Valid
          (Actor|DestroyActor))))
    (:Finished
      (Default|SetPartActive/Deactive (Variables|Default|GetInBuildActor) (Variables|Default|GetInStatic%20Mesh) true)
      (CallFunction|DestroySelf))))

(event Custom|DestroySelf
  (Utilities|FlowControl|Delay 0.5)
  (Actor|DestroyActor))

(event EventBeginPlay
  (Utilities|IsValid (Variables|Default|GetInStatic%20Mesh)
    (:Is%20Valid
      (Components|StaticMesh|SetStaticMesh (Variables|Default|GetStaticMesh) (Variables|/Script/Engine.StaticMeshComponent|GetStaticMesh (Variables|Default|GetInStatic%20Mesh)))
      (CallFunction|SetTextures)
      (Utilities|FlowControl|Delay 0.01)
      (CallFunction|DynamiclyAdd)
      (Audio|Components|Audio|Play (Variables|Default|GetAudio) (Math|Random|RandomFloatinRange 0.0 5.0))
      (Utilities|FlowControl|Delay 1.2)
      (Audio|Components|Audio|FadeOut (Variables|Default|GetAudio) 0.4 0.0 "Linear" :!class /Script/Engine.AudioComponent))
    (:Is%20Not%20Valid
      (Actor|DestroyActor))))

(fn ConstructionScript)

(fn SetTextures
  (for _index (range 0 (- (Rendering|Material|GetNumMaterials (Variables|Default|GetStaticMesh)) 1))
    (Rendering|Material|SetMaterial (Variables|Default|GetStaticMesh) _index (.Value (Utilities|Map|Find (Variables|Default|GetMaterials) _index))))
  (return))