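; Buildable wooden door that toggles open and closed on interaction and registers its parts for destruction.
; A timeline played forward or in reverse swings the main mesh, with IsActive blocking interaction during motion.
; The prompt text toggles, hides during the swing, then returns at the knob if InSphere is true.
; AddMesh fills the mesh list and maps each mesh to a geometry collection for destruction.
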(event EventBeginPlay
  (|CallParentFunction) ; This node is disabled and will not be called.\nDrag off pins to build functionality.
)

(event EventInteractStart
  (if (not (Variables|Default|GetIsActive))
    (if (not (Variables|Default|GetIsOppen))
      (Variables|Default|SetIsOppen true)
      (Variables|/Script/UMG.TextBlock|SetText (Variables|Default|GetText) "Close Door")
      (bind _oppenclose (Timeline|Timeline PlayFromStart)
        (:Update
          (Variables|Default|SetIsActive true)
          (Transformation|SetRelativeRotation (Variables|Default|GetStaticMesh) (Math|Rotator|Lerp(Rotator) "0, 0, 0" "0.000000,100.000000,0.000000" _oppenclose) false false)
          (Rendering|SetVisibility (Variables|Default|GetInteractText) false false))
        (:Finished
          (Variables|Default|SetIsActive false)
          (if (Variables|Default|GetInSphere)
            (Rendering|SetVisibility (Variables|Default|GetInteractText) true false)
            (Transformation|SetWorldLocation (Variables|Default|GetInteractText) (Transformation|GetWorldLocation (Variables|Default|GetDoorNobLocation)) false false))))
      (else
        (Variables|Default|SetIsOppen false)
        (Variables|/Script/UMG.TextBlock|SetText (Variables|Default|GetText) "Open Door")
        (Timeline|Timeline ReverseFromEnd)))))

(fn ConstructionScript
  (|CallParentFunction))

(fn AddMesh
  (Variables|Default|SetAllMesh (Utilities|Array|MakeArray (Variables|Default|GetWoodDoor_2_) (Variables|Default|GetStaticMesh) (Variables|Default|GetWoodDoor_3_) (Variables|Default|GetWoodDoor_4_) (Variables|Default|GetWoodDoor_5_) (Variables|Default|GetWoodDoor_6_) (Variables|Default|GetWoodDoor_7_) (Variables|Default|GetWoodDoor_8_)))
  (Utilities|Map|Add (Variables|Default|GetMeshToDestructionMesh) (Variables|Default|GetStaticMesh) (Variables|Default|Getfoundation_GeometryCollection))
  (Utilities|Map|Add (Variables|Default|GetMeshToDestructionMesh) (Variables|Default|GetWoodDoor_2_) (Variables|Default|GetWoodDoor_2_GeometryCollection))
  (Utilities|Map|Add (Variables|Default|GetMeshToDestructionMesh) (Variables|Default|GetWoodDoor_3_) (Variables|Default|GetWoodDoor_3_GeometryCollection))
  (Utilities|Map|Add (Variables|Default|GetMeshToDestructionMesh) (Variables|Default|GetWoodDoor_4_) (Variables|Default|GetWoodDoor_4_GeometryCollection))
  (Utilities|Map|Add (Variables|Default|GetMeshToDestructionMesh) (Variables|Default|GetWoodDoor_5_) (Variables|Default|GetWoodDoor_5__GeometryCollection))
  (Utilities|Map|Add (Variables|Default|GetMeshToDestructionMesh) (Variables|Default|GetWoodDoor_6_) (Variables|Default|GetWoodDoor_6_GeometryCollection))
  (Utilities|Map|Add (Variables|Default|GetMeshToDestructionMesh) (Variables|Default|GetWoodDoor_7_) (Variables|Default|GetWoodDoor_7_GeometryCollection))
  (Utilities|Map|Add (Variables|Default|GetMeshToDestructionMesh) (Variables|Default|GetWoodDoor_8_) (Variables|Default|GetWoodDoor_8_GeometryCollection)))