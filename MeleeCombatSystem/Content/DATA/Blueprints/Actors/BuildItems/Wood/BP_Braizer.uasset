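; BP_Braizer is a wooden build item, a brazier that the player can light and put out through interaction.
; InteractStart toggles IsOppen, switching the prompt text and the fire particle system and point light, while Deactivate forces the put-out branch.
; AddMesh lists its meshes and maps the static mesh to a geometry collection for destruction.
; A rotation timeline remains in the graph but is never triggered.
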(event EventBeginPlay
  (|CallParentFunction) ; This node is disabled and will not be called.\nDrag off pins to build functionality.
)

(event EventDeactivate
  (Variables|Default|SetIsOppen false)
  (Variables|/Script/UMG.TextBlock|SetText (Variables|Default|GetText) "Light")
  (Components|Activation|Deactivate (Variables|Default|GetParticleSystem))
  (Rendering|SetVisibility (Variables|Default|GetPointLight) false false))

(event EventInteractStart
  (if (not (Variables|Default|GetIsActive))
    (if (not (Variables|Default|GetIsOppen))
      (Variables|Default|SetIsOppen true)
      (Variables|/Script/UMG.TextBlock|SetText (Variables|Default|GetText) "Put Out")
      (Components|Activation|Activate (Variables|Default|GetParticleSystem) false)
      (Rendering|SetVisibility (Variables|Default|GetPointLight) true false)
      (else
        (Variables|Default|SetIsOppen false)
        (Variables|/Script/UMG.TextBlock|SetText (Variables|Default|GetText) "Light")
        (Components|Activation|Deactivate (Variables|Default|GetParticleSystem))
        (Rendering|SetVisibility (Variables|Default|GetPointLight) false false)))))

(fn ConstructionScript
  (|CallParentFunction))

(fn AddMesh
  (Variables|Default|SetAllMesh (Utilities|Array|MakeArray (Variables|Default|GetStaticMesh) (Variables|Default|GetWoodShards)))
  (Utilities|Map|Add (Variables|Default|GetMeshToDestructionMesh) (Variables|Default|GetStaticMesh) (Variables|Default|Getfoundation_GeometryCollection)))