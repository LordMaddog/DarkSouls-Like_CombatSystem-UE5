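; Wooden floor piece for the building system, assembled from four static meshes.
; BuildSnapLoc returns snap data for its north, south, east and west boxes, choosing each scene location by whether a foundation, wall or floor is being placed.
; AddMesh registers the meshes and maps each one to a Geometry Collection as its destruction counterpart.
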(event EventBeginPlay
  (|CallParentFunction) ; This node is disabled and will not be called.\nDrag off pins to build functionality.
)

(fn ConstructionScript
  (|CallParentFunction))

(fn BuildSnapLoc
  (params (BuildType :type E_BuildType%20Enum :default "NewEnumerator0") (BuildSize :type E_BuildSize%20Enum :default "NewEnumerator0"))
  (return (Utilities|Array|MakeArray (Utilities|Struct|MakeS_BuildSnapLoc (Variables|Default|GetNorthBox) (Utilities|Select :Index BuildType :NewEnumerator0 0 :NewEnumerator1 (Variables|Default|GetNorthFoundationLoc) :NewEnumerator2 (Variables|Default|GetNorthwallLoc) :NewEnumerator3 0 :NewEnumerator4 0 :NewEnumerator5 (Variables|Default|GetNorthFloorLoc))) (Utilities|Struct|MakeS_BuildSnapLoc (Variables|Default|GetSouthBox) (Utilities|Select :Index BuildType :NewEnumerator0 0 :NewEnumerator1 (Variables|Default|GetSouthFoundationLoc) :NewEnumerator2 (Variables|Default|GetSouthwallLoc) :NewEnumerator3 0 :NewEnumerator4 0 :NewEnumerator5 (Variables|Default|GetSouthFloorLoc))) (Utilities|Struct|MakeS_BuildSnapLoc (Variables|Default|GetEastBox) (Utilities|Select :Index BuildType :NewEnumerator0 0 :NewEnumerator1 (Variables|Default|GetEastFoundationLoc) :NewEnumerator2 (Variables|Default|GetEastwallLoc) :NewEnumerator3 0 :NewEnumerator4 0 :NewEnumerator5 (Variables|Default|GetEastFloorLoc))) (Utilities|Struct|MakeS_BuildSnapLoc (Variables|Default|GetWestBox) (Utilities|Select :Index BuildType :NewEnumerator0 0 :NewEnumerator1 (Variables|Default|GetWestFoundationLoc) :NewEnumerator2 (Variables|Default|GetWestwallLoc) :NewEnumerator3 0 :NewEnumerator4 0 :NewEnumerator5 (Variables|Default|GetWestFloorLoc))))))

(fn AddMesh
  (Variables|Default|SetAllMesh (Utilities|Array|MakeArray (Variables|Default|GetStaticMesh) (Variables|Default|GetWood_floor_ceiling_2_) (Variables|Default|GetWood_floor_ceiling_3_) (Variables|Default|GetWood_floor_ceiling_4_)))
  (Utilities|Map|Add (Variables|Default|GetMeshToDestructionMesh) (Variables|Default|GetStaticMesh) (Variables|Default|Getfoundation_GeometryCollection))
  (Utilities|Map|Add (Variables|Default|GetMeshToDestructionMesh) (Variables|Default|GetWood_floor_ceiling_2_) (Variables|Default|GetWood_floor_ceiling_2_GeometryCollection))
  (Utilities|Map|Add (Variables|Default|GetMeshToDestructionMesh) (Variables|Default|GetWood_floor_ceiling_3_) (Variables|Default|GetWood_floor_ceiling_3_GeometryCollection))
  (Utilities|Map|Add (Variables|Default|GetMeshToDestructionMesh) (Variables|Default|GetWood_floor_ceiling_4_) (Variables|Default|GetWood_floor_ceiling_4_GeometryCollection)))