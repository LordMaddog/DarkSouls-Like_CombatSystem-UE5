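; Wooden foundation extension build item, made of twelve static mesh pieces.
; AddMesh fills AllMesh with the pieces and maps each one to its own geometry collection in MeshToDestructionMesh, pairing every mesh with a destruction counterpart.
; The event graph is unused and the construction script only calls the parent.
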(event EventBeginPlay
  (|CallParentFunction) ; This node is disabled and will not be called.\nDrag off pins to build functionality.
)

(event Collision|EventActorBeginOverlap
  (params (OtherActor :type Actor%20Object%20Reference)))

(event EventTick
  (params (DeltaSeconds :type Float%20%28single-precision%29)))

(fn ConstructionScript
  (|CallParentFunction))

(fn AddMesh
  (Variables|Default|SetAllMesh (Utilities|Array|MakeArray (Variables|Default|GetStaticMesh) (Variables|Default|Getfoundation_extention_2_) (Variables|Default|Getfoundation_extention_3_) (Variables|Default|Getfoundation_extention_4_) (Variables|Default|Getfoundation_extention_5_) (Variables|Default|Getfoundation_extention_6_) (Variables|Default|Getfoundation_extention_7_) (Variables|Default|Getfoundation_extention_8_) (Variables|Default|Getfoundation_extention_9_) (Variables|Default|Getfoundation_extention_10_) (Variables|Default|Getfoundation_extention_11_) (Variables|Default|Getfoundation_extention_12_)))
  (Utilities|Map|Add (Variables|Default|GetMeshToDestructionMesh) (Variables|Default|GetStaticMesh) (Variables|Default|Getfoundation_GeometryCollection))
  (Utilities|Map|Add (Variables|Default|GetMeshToDestructionMesh) (Variables|Default|Getfoundation_extention_2_) (Variables|Default|Getfoundation_extention_2_GeometryCollection))
  (Utilities|Map|Add (Variables|Default|GetMeshToDestructionMesh) (Variables|Default|Getfoundation_extention_3_) (Variables|Default|Getfoundation_extention_3_GeometryCollection))
  (Utilities|Map|Add (Variables|Default|GetMeshToDestructionMesh) (Variables|Default|Getfoundation_extention_4_) (Variables|Default|Getfoundation_extention_4_GeometryCollection))
  (Utilities|Map|Add (Variables|Default|GetMeshToDestructionMesh) (Variables|Default|Getfoundation_extention_5_) (Variables|Default|Getfoundation_extention_5_GeometryCollection))
  (Utilities|Map|Add (Variables|Default|GetMeshToDestructionMesh) (Variables|Default|Getfoundation_extention_6_) (Variables|Default|Getfoundation_extention_6_GeometryCollection))
  (Utilities|Map|Add (Variables|Default|GetMeshToDestructionMesh) (Variables|Default|Getfoundation_extention_7_) (Variables|Default|Getfoundation_extention_7_GeometryCollection))
  (Utilities|Map|Add (Variables|Default|GetMeshToDestructionMesh) (Variables|Default|Getfoundation_extention_8_) (Variables|Default|Getfoundation_extention_8_GeometryCollection))
  (Utilities|Map|Add (Variables|Default|GetMeshToDestructionMesh) (Variables|Default|Getfoundation_extention_9_) (Variables|Default|Getfoundation_extention_9_GeometryCollection))
  (Utilities|Map|Add (Variables|Default|GetMeshToDestructionMesh) (Variables|Default|Getfoundation_extention_10_) (Variables|Default|Getfoundation_extention_10_GeometryCollection))
  (Utilities|Map|Add (Variables|Default|GetMeshToDestructionMesh) (Variables|Default|Getfoundation_extention_11_) (Variables|Default|Getfoundation_extention_11_GeometryCollection))
  (Utilities|Map|Add (Variables|Default|GetMeshToDestructionMesh) (Variables|Default|Getfoundation_extention_12_) (Variables|Default|Getfoundation_extention_12_GeometryCollection)))