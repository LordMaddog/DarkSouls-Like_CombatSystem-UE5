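; Wooden foundation build piece for the building system, a child that supplies its own snap points and meshes.
; BuildSnapLoc pairs four side boxes with foundation, wall or floor scene locations chosen by build type, plus a center box with no location.
; AddMesh registers the piece's static meshes and maps each to a geometry collection for destruction.
; BeginPlay gathers the four diagonal arrow components into an array.
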(event EventBeginPlay
  (|CallParentFunction)
  (Variables|Default|SetArrows (Utilities|Array|MakeArray (Variables|Default|GetNEArrow) (Variables|Default|GetSWArrow) (Variables|Default|GetNWArrow) (Variables|Default|GetSEArrow))))

(fn ConstructionScript
  (|CallParentFunction))

(fn BuildSnapLoc
  (params (BuildType :type E_BuildType%20Enum :default "NewEnumerator0") (BuildSize :type E_BuildSize%20Enum :default "NewEnumerator0"))
  (return (Utilities|Array|MakeArray (Utilities|Struct|MakeS_BuildSnapLoc (Variables|Default|GetNorthBox) (Utilities|Select :Index BuildType :NewEnumerator0 0 :NewEnumerator1 (Variables|Default|GetNorthFoundationLoc) :NewEnumerator2 (Variables|Default|GetNorthwallLoc) :NewEnumerator3 0 :NewEnumerator4 0 :NewEnumerator5 (Variables|Default|GetNorthFloorLoc))) (Utilities|Struct|MakeS_BuildSnapLoc (Variables|Default|GetSouthBox) (Utilities|Select :Index BuildType :NewEnumerator0 0 :NewEnumerator1 (Variables|Default|GetSouthFoundationLoc) :NewEnumerator2 (Variables|Default|GetSouthwallLoc) :NewEnumerator3 0 :NewEnumerator4 0 :NewEnumerator5 (Variables|Default|GetSouthFloorLoc))) (Utilities|Struct|MakeS_BuildSnapLoc (Variables|Default|GetEastBox) (Utilities|Select :Index BuildType :NewEnumerator0 0 :NewEnumerator1 (Variables|Default|GetEastFoundationLoc) :NewEnumerator2 (Variables|Default|GetEastwallLoc) :NewEnumerator3 0 :NewEnumerator4 0 :NewEnumerator5 (Variables|Default|GetEastFloorLoc))) (Utilities|Struct|MakeS_BuildSnapLoc (Variables|Default|GetWestBox) (Utilities|Select :Index BuildType :NewEnumerator0 0 :NewEnumerator1 (Variables|Default|GetWestFoundationLoc) :NewEnumerator2 (Variables|Default|GetWestwallLoc) :NewEnumerator3 0 :NewEnumerator4 0 :NewEnumerator5 (Variables|Default|GetWestFloorLoc))) (Utilities|Struct|MakeS_BuildSnapLoc (Variables|Default|GetCenterBox) (Utilities|Select :Index BuildType :NewEnumerator0 0 :NewEnumerator1 0 :NewEnumerator2 0 :NewEnumerator3 0 :NewEnumerator4 0 :NewEnumerator5 0)))))

(fn AddMesh
  (Variables|Default|SetAllMesh (Utilities|Array|MakeArray (Variables|Default|GetStaticMesh) (Variables|Default|Getfoundation_GeometryCollection_SM_7_) (Variables|Default|Getfoundation_GeometryCollection_SM_11_) (Variables|Default|Getfoundation_GeometryCollection_SM_6_) (Variables|Default|Getfoundation_GeometryCollection_SM_9_) (Variables|Default|Getfoundation_GeometryCollection_SM_8_) (Variables|Default|Getfoundation_GeometryCollection_SM_1_) (Variables|Default|Getfoundation_GeometryCollection_SM_5_) (Variables|Default|Getfoundation_GeometryCollection_SM_12_) (Variables|Default|Getfoundation_GeometryCollection_SM_4_) (Variables|Default|Getfoundation_GeometryCollection_SM_3_) (Variables|Default|Getfoundation_GeometryCollection_SM_2_)))
  (Utilities|Map|Add (Variables|Default|GetMeshToDestructionMesh) (Variables|Default|Getfoundation_GeometryCollection_SM_1_) (Variables|Default|Getfoundation_GeometryCollection_SM_1__GeometryCollection))
  (Utilities|Map|Add (Variables|Default|GetMeshToDestructionMesh) (Variables|Default|Getfoundation_GeometryCollection_SM_2_) (Variables|Default|Getfoundation_GeometryCollection_SM_2__GeometryCollection))
  (Utilities|Map|Add (Variables|Default|GetMeshToDestructionMesh) (Variables|Default|Getfoundation_GeometryCollection_SM_3_) (Variables|Default|Getfoundation_GeometryCollection_SM_3__GeometryCollection))
  (Utilities|Map|Add (Variables|Default|GetMeshToDestructionMesh) (Variables|Default|Getfoundation_GeometryCollection_SM_4_) (Variables|Default|Getfoundation_GeometryCollection_SM_4__GeometryCollection))
  (Utilities|Map|Add (Variables|Default|GetMeshToDestructionMesh) (Variables|Default|Getfoundation_GeometryCollection_SM_5_) (Variables|Default|Getfoundation_GeometryCollection_SM_5__GeometryCollection))
  (Utilities|Map|Add (Variables|Default|GetMeshToDestructionMesh) (Variables|Default|Getfoundation_GeometryCollection_SM_6_) (Variables|Default|Getfoundation_GeometryCollection_SM_6__GeometryCollection))
  (Utilities|Map|Add (Variables|Default|GetMeshToDestructionMesh) (Variables|Default|Getfoundation_GeometryCollection_SM_7_) (Variables|Default|Getfoundation_GeometryCollection_SM_7__GeometryCollection))
  (Utilities|Map|Add (Variables|Default|GetMeshToDestructionMesh) (Variables|Default|Getfoundation_GeometryCollection_SM_8_) (Variables|Default|Getfoundation_GeometryCollection_SM_8__GeometryCollection))
  (Utilities|Map|Add (Variables|Default|GetMeshToDestructionMesh) (Variables|Default|Getfoundation_GeometryCollection_SM_9_) (Variables|Default|Getfoundation_GeometryCollection_SM_9__GeometryCollection))
  (Utilities|Map|Add (Variables|Default|GetMeshToDestructionMesh) (Variables|Default|GetStaticMesh) (Variables|Default|Getfoundation_GeometryCollection))
  (Utilities|Map|Add (Variables|Default|GetMeshToDestructionMesh) (Variables|Default|Getfoundation_GeometryCollection_SM_11_) (Variables|Default|Getfoundation_GeometryCollection_SM_11__GeometryCollection))
  (Utilities|Map|Add (Variables|Default|GetMeshToDestructionMesh) (Variables|Default|Getfoundation_GeometryCollection_SM_12_) (Variables|Default|Getfoundation_GeometryCollection_SM_12__GeometryCollection)))