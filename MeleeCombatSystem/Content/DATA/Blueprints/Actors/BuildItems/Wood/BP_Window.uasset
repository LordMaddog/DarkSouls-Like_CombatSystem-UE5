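; Wooden window build item that the player can interact with to open and close.
; InteractStart toggles the state and plays or reverses a timeline that swings the two meshes in opposite directions, ignoring input while animating.
; The prompt label switches between open and close, hiding during motion and returning if InSphere is set.
; AddMesh registers both meshes and maps each to a geometry collection for destruction.
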(event EventBeginPlay
  (|CallParentFunction))

(event EventInteractStart
  (if (not (Variables|Default|GetIsActive))
    (if (not (Variables|Default|GetIsOppen))
      (Variables|Default|SetIsOppen true)
      (Variables|/Script/UMG.TextBlock|SetText (Variables|Default|GetText) "Close Window")
      (bind _oppenclose (Timeline|Timeline PlayFromStart)
        (:Update
          (Variables|Default|SetIsActive true)
          (Transformation|SetRelativeRotation (Variables|Default|GetStaticMesh) (Math|Rotator|Lerp(Rotator) "0.000000,180.000000,0.000000" "0.000000,80.000000,0.000000" _oppenclose) false false)
          (Transformation|SetRelativeRotation (Variables|Default|GetStaticMesh1_0) (Math|Rotator|Lerp(Rotator) "0, 0, 0" "0.000000,100.000000,0.000000" _oppenclose) false false)
          (Rendering|SetVisibility (Variables|Default|GetInteractText) false false))
        (:Finished
          (Variables|Default|SetIsActive false)
          (if (Variables|Default|GetInSphere)
            (Rendering|SetVisibility (Variables|Default|GetInteractText) true false))))
      (else
        (Variables|Default|SetIsOppen false)
        (Variables|/Script/UMG.TextBlock|SetText (Variables|Default|GetText) "Oppen Window")
        (Timeline|Timeline ReverseFromEnd)))))

(fn ConstructionScript
  (|CallParentFunction))

(fn AddMesh
  (Variables|Default|SetAllMesh (Utilities|Array|MakeArray (Variables|Default|GetStaticMesh) (Variables|Default|GetStaticMesh1_0)))
  (Utilities|Map|Add (Variables|Default|GetMeshToDestructionMesh) (Variables|Default|GetStaticMesh) (Variables|Default|Getfoundation_GeometryCollection))
  (Utilities|Map|Add (Variables|Default|GetMeshToDestructionMesh) (Variables|Default|GetStaticMesh1_0) (Variables|Default|Getwindows_GeometryCollection)))