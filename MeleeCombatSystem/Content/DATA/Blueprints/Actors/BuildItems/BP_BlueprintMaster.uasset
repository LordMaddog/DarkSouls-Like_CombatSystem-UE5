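; Blueprint tool actor for saving groups of player builds as named blueprints and placing copies of them.
; An adjustable box selects and highlights builds, which are saved to per-name SaveGame slots, with a shared metadata slot holding name, date and screenshot icon.
; Loading spawns collision-disabled previews attached to this actor.
; CanBuild box-traces and tints each piece for validity, and Place detaches them, adding foundation extensions to certain types.
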(event Custom|SelectBuilds
  ;[1 1 1] Select Builds to save
  (for _array_element (Collision|GetOverlappingActors (Variables|Default|GetBox) "/Game/DATA/Blueprints/Actors/BuildItems/BP_MasterBuild.BP_MasterBuild_C" :!class /Script/Engine.PrimitiveComponent)
    (bind _builditem (Class|BuildBPI|GetBuildItem(Message) _array_element))
    (Utilities|IsValid _builditem
      (:Is%20Valid
        (if (not (Utilities|Array|ContainsItem (Variables|Default|GetSelected%20Builds) _builditem))
          (Utilities|Array|Add (Variables|Default|GetSelected%20Builds) _builditem)
          (Default|HighlightonOff _builditem true))))))

(event Custom|AdjustBoxExtent
  (params (AddExtent :type Vector))
  (bind _box (Variables|Default|GetBox))
  ;[1 1 1] Change Selection Size
  (Components|Box|SetBoxExtent _box (+ AddExtent (Variables|/Script/Engine.BoxComponent|GetBoxExtent _box)) false))

(event Custom|BeginSave
  (bind (_widget_place_x _widget_place_y) (CallFunction|GetViewportCenter))
  ;[1 1 1] Start Saving blue print
  (Utilities|FlowControl|Delay 0.1)
  (CallFunction|RemoveUI)
  (bind _returnvalue (UserInterface|CreateWidget "/Game/DATA/UI/Menus/Sub/CW_SaveBlueprintMenu.CW_SaveBlueprintMenu_C" (Variables|/Game/DATA/BP_BuildPawn.BP_BuildPawn_C|GetPlayer%20Controller (Variables|Default|GetPlayer))))
  (Variables|Default|SetSaveMenu _returnvalue)
  (Variables|/Game/DATA/UI/Menus/Sub/CW_SaveBlueprintMenu.CW_SaveBlueprintMenu_C|SetMasterBlueprint _returnvalue self)
  (CallFunction|TakeSaveIconScreenShotCalled "temp")
  (Utilities|FlowControl|Delay 0.2)
  (bind _returnvalue_2 (CallFunction|GetSaveIcon "temp"))
  (Default|SetSaveIcon _returnvalue _returnvalue_2)
  (Class|UserWidget|SetDesiredSizeinViewport (Variables|Default|GetSaveMenu) "(X=700.000000,Y=466.600000)")
  (Class|UserWidget|SetAlignmentinViewport (Variables|Default|GetSaveMenu) "(X=0.500000,Y=0.500000)")
  (Class|UserWidget|SetPositioninViewport (Variables|Default|GetSaveMenu) (Math|Vector2D|MakeVector2D _widget_place_x _widget_place_y) true)
  (UserInterface|Viewport|AddtoViewport (Variables|Default|GetSaveMenu) 0)
  (Class|CombatBPI|ToggleMouseCursor(Message) (Variables|/Game/DATA/BP_BuildPawn.BP_BuildPawn_C|GetPlayer%20Controller (Variables|Default|GetPlayer))))

(event Custom|SaveBlueprint
  (params (Save%20Name :type String))
  ;[1 1 1] Save Blueprint
  (CallFunction|AddMetaData Save%20Name)
  (Variables|Default|GetSavedBlueprint
    (:then
      _)
    (:else
      (bind _returnvalue (SaveGame|CreateSaveGameObject "/Game/DATA/Blueprints/SaveGame/BP_BuildBlueprintSave.BP_BuildBlueprintSave_C"))
      (Variables|Default|SetSavedBlueprint _returnvalue)))
  (Default|SaveBluePrint (Variables|Default|GetSavedBlueprint) (Variables|Default|GetSelected%20Builds))
  (bind _returnvalue_2 (SaveGame|SaveGametoSlot (Variables|Default|GetSavedBlueprint) (Utilities|String|Append "BluePrint-" Save%20Name)))
  (if _returnvalue_2
    (CallFunction|ClearSelection)
    (Widget|RemovefromParent (Variables|Default|GetSaveMenu))
    (Class|CombatBPI|ToggleMouseCursor(Message) (Variables|/Game/DATA/BP_BuildPawn.BP_BuildPawn_C|GetPlayer%20Controller (Variables|Default|GetPlayer)))
    (Default|StopBuildMode (Variables|/Game/DATA/BP_BuildPawn.BP_BuildPawn_C|GetBuildComponent (Variables|Default|GetPlayer)))))

(event Custom|CancelSave
  ;[1 1 1] Abort save
  (Class|CombatBPI|ToggleMouseCursor(Message) (Variables|/Game/DATA/BP_BuildPawn.BP_BuildPawn_C|GetPlayer%20Controller (Variables|Default|GetPlayer)))
  (Widget|RemovefromParent (Variables|Default|GetSaveMenu)))

(event Custom|StartLoad
  (bind (_widget_place_x _widget_place_y) (CallFunction|GetViewportCenter))
  ;[1 1 1] Start Load
  (Utilities|FlowControl|Delay 0.1)
  (CallFunction|RemoveUI)
  (bind _returnvalue (UserInterface|CreateWidget "/Game/DATA/UI/Menus/Sub/CW_LoadBlueprintMenu.CW_LoadBlueprintMenu_C"))
  (Variables|Default|SetBlueprintMenu _returnvalue)
  (Default|OppenLoadMenu (Variables|Default|GetBlueprintMenu) self)
  (Class|UserWidget|SetAlignmentinViewport (Variables|Default|GetBlueprintMenu) "(X=0.500000,Y=0.500000)")
  (Class|UserWidget|SetPositioninViewport (Variables|Default|GetBlueprintMenu) (Math|Vector2D|MakeVector2D _widget_place_x _widget_place_y) true)
  (UserInterface|Viewport|AddtoViewport (Variables|Default|GetBlueprintMenu) 0)
  (Class|CombatBPI|ToggleMouseCursor(Message) (Variables|/Game/DATA/BP_BuildPawn.BP_BuildPawn_C|GetPlayer%20Controller (Variables|Default|GetPlayer))))

(event Custom|Load
  (params (SlotName :type String))
  ;[1 1 1] Load
  (bind _returnvalue (SaveGame|LoadGamefromSlot (Utilities|String|Append "BluePrint-" SlotName)))
  (bind _asbp_build_blueprint_save (Utilities|Casting|CastToBP_BuildBlueprintSave _returnvalue))
  (Variables|Default|SetSavedBlueprint _asbp_build_blueprint_save)
  (Widget|RemovefromParent (Variables|Default|GetBlueprintMenu))
  (Class|CombatBPI|ToggleMouseCursor(Message) (Variables|/Game/DATA/BP_BuildPawn.BP_BuildPawn_C|GetPlayer%20Controller (Variables|Default|GetPlayer)))
  (Variables|Default|SetSpawning true)
  (Transformation|SetActorLocation (.Location (Math|Transform|BreakTransform (.Transform (Utilities|Struct|BreakS_BuildItemsSave (Utilities|Array|Get(acopy) (Variables|/Game/DATA/Blueprints/SaveGame/BP_BuildBlueprintSave.BP_BuildBlueprintSave_C|GetBuildItemSave (Variables|Default|GetSavedBlueprint))))))) false false)
  (Rendering|SetVisibility (Variables|Default|GetBox) false false)
  (for _array_element (Variables|/Game/DATA/Blueprints/SaveGame/BP_BuildBlueprintSave.BP_BuildBlueprintSave_C|GetBuildItemSave (Variables|Default|GetSavedBlueprint))
    (bind _returnvalue_2 (Game|SpawnActorfromClass (.class _array_element) (.transform _array_element) "Undefined" "MultiplyWithRoot" 0 false (.buildsize _array_element) false true false 0))
    (Default|DisableAllColision _returnvalue_2)
    (Default|GiveBuildColor _returnvalue_2 true)
    (Utilities|Array|Add (Variables|Default|GetBuildArray) _returnvalue_2)
    (Transformation|AttachActorToActor _returnvalue_2 self "None" "KeepWorld" "KeepWorld" "KeepWorld" true)))

(event Custom|LoadCancel
  ;[1 1 1] Abort Load
  (Widget|RemovefromParent (Variables|Default|GetBlueprintMenu))
  (Class|CombatBPI|ToggleMouseCursor(Message) (Variables|/Game/DATA/BP_BuildPawn.BP_BuildPawn_C|GetPlayer%20Controller (Variables|Default|GetPlayer))))

(event EventBeginPlay
  ;[1 1 1] Event begin player Load blueprint meta data
  (bind _returnvalue (SaveGame|LoadGamefromSlot "SaveBluePrintMeta"))
  (bind _asbp_save_meta_data (Utilities|Casting|CastToBP_SaveMetaData _returnvalue)
    (:then
      (Variables|Default|SetSaveMeta _asbp_save_meta_data))
    (:CastFailed
      (bind _returnvalue_2 (SaveGame|CreateSaveGameObject "/Game/DATA/Blueprints/SaveGame/BP_SaveMetaData.BP_SaveMetaData_C"))
      (bind _output_get (Variables|Default|SetSaveMeta _returnvalue_2))
      (SaveGame|SaveGametoSlot _output_get "SaveBluePrintMeta")))
  (CallFunction|LoadtheMetaData))

(fn ConstructionScript)

(fn SavetheMetaData
  (Utilities|IsValid (Variables|Default|GetSaveMeta)
    (:Is%20Valid
      _)
    (:Is%20Not%20Valid
      (bind _returnvalue (SaveGame|CreateSaveGameObject "/Game/DATA/Blueprints/SaveGame/BP_SaveMetaData.BP_SaveMetaData_C"))
      (Variables|Default|SetSaveMeta _returnvalue)))
  (Variables|/Game/DATA/Blueprints/SaveGame/BP_SaveMetaData.BP_SaveMetaData_C|SetSaveMetaData (Variables|Default|GetSaveMeta) (Variables|Default|GetSaveMetaData))
  (SaveGame|SaveGametoSlot (Variables|Default|GetSaveMeta) "SaveBluePrintMeta"))

(fn LoadtheMetaData
  (Variables|Default|SetSaveMetaData (Variables|/Game/DATA/Blueprints/SaveGame/BP_SaveMetaData.BP_SaveMetaData_C|GetSaveMetaData (Variables|Default|GetSaveMeta))))

(fn TakeSaveIconScreenShot
  (params (Filename :type String))
  (Game|SpawnActorfromClass "/Game/DATA/Blueprints/Actors/Utility/BP_SaveScreenshotCamera.BP_SaveScreenshotCamera_C" (Transformation|GetWorldTransform (Variables|/Game/DATA/BP_BuildPawn.BP_BuildPawn_C|GetCamera (Variables|Default|GetPlayer))) "Undefined" "MultiplyWithRoot" 0 0)
  (Class|AutomationBlueprintFunctionLibrary|TakeHighResScreenshot 960 540 (Utilities|String|Append (Class|BlueprintPathsLibrary|ProjectSavedDir) "/SaveGames/Screenshots/" Filename) 0 false false "Low" "" 0.0)
  (bind _returnvalue (Class|KismetRenderingLibrary|ImportFileasTexture2D (Utilities|String|Append (Class|BlueprintPathsLibrary|ProjectSavedDir) "/SaveGames/Screenshots/" Filename ".png")))
  (return _returnvalue))

(fn AddMetaData
  (params (Save%20Name :type String))
  (bind _returnvalue (Math|DateTime|Now))
  (LocalVariables|SetIndexToDelete -1)
  (for (_array_element _array_index) (Variables|Default|GetSaveMetaData)
    (if (Utilities|Enum|Equal(Enum) (.savename _array_element) Save%20Name)
      (LocalVariables|SetIndexToDelete _array_index)))
  (if (>= (LocalVariables|GetIndexToDelete) 0)
    (Utilities|Array|RemoveIndex (Variables|Default|GetSaveMetaData) (LocalVariables|GetIndexToDelete)))
  (Utilities|Array|AddUnique (Variables|Default|GetSaveMetaData) (Utilities|Struct|MakeSaveMeta Save%20Name (Utilities|String|Append (Utilities|String|ToString(Integer) (.month _returnvalue)) "/" (Utilities|String|ToString(Integer) (.day _returnvalue)) "/" (Utilities|String|ToString(Integer) (.year _returnvalue)) "   " (Utilities|String|ToString(Integer) (.hour _returnvalue)) ":" (Utilities|String|ToString(Integer) (.minute _returnvalue))) (+ (Utilities|Array|Length (Variables|Default|GetSaveMetaData)) 1) (CallFunction|TakeSaveIconScreenShot Save%20Name)))
  (CallFunction|SavetheMetaData))

(fn ClearSelection
  (for _array_element (Variables|Default|GetSelected%20Builds)
    (Default|HighlightonOff _array_element false))
  (Utilities|Array|Clear (Variables|Default|GetSelected%20Builds)))

(fn GetSaveIcon
  (params (Filename :type String))
  (bind _returnvalue (Class|KismetRenderingLibrary|ImportFileasTexture2D (Utilities|String|Append (Class|BlueprintPathsLibrary|ProjectSavedDir) "/SaveGames/Screenshots/" Filename ".png")))
  (return _returnvalue))

(fn TakeSaveIconScreenShotCalled
  (params (Filename :type String))
  (Game|SpawnActorfromClass "/Game/DATA/Blueprints/Actors/Utility/BP_SaveScreenshotCamera.BP_SaveScreenshotCamera_C" (Transformation|GetWorldTransform (Variables|/Game/DATA/BP_BuildPawn.BP_BuildPawn_C|GetCamera (Variables|Default|GetPlayer))) "Undefined" "MultiplyWithRoot" 0 0)
  (Class|AutomationBlueprintFunctionLibrary|TakeHighResScreenshot 960 540 (Utilities|String|Append (Class|BlueprintPathsLibrary|ProjectSavedDir) "/SaveGames/Screenshots/" Filename) 0 false false "Low" "" 0.0)
  (bind _returnvalue (Class|KismetRenderingLibrary|ImportFileasTexture2D (Utilities|String|Append (Class|BlueprintPathsLibrary|ProjectSavedDir) "/SaveGames/Screenshots/" Filename ".png")))
  (return _returnvalue))

(fn GetWidgetinCenter
  (params (Widget%20size%20X :type Float%20%28double-precision%29) (Widget%20size%20Y :type Float%20%28double-precision%29))
  (bind _returnvalue (Viewport|GetViewportSize))
  (return (- (/ (.x _returnvalue) 2.0) (/ Widget%20size%20X 2.0)) (- (/ (.y _returnvalue) 2.0) (/ Widget%20size%20Y 2.0))))

(fn GetViewportCenter
  (bind _returnvalue (Viewport|GetViewportSize))
  (return (/ (.x _returnvalue) 2.0) (/ (.y _returnvalue) 2.0)))

(fn DestroySpawned
  (for _array_element (Variables|Default|GetBuildArray)
    (Actor|DestroyActor _array_element)))

(fn ChechforOverlap
  (params (Target :type BP%20Master%20Build%20Object%20Reference))
  (bind _collisioncheckmesh (Variables|/Game/DATA/Blueprints/Actors/BuildItems/BP_MasterBuild.BP_MasterBuild_C|GetCollisionCheckMesh Target))
  (bind (_origin _boxextent) (Collision|GetComponentBounds _collisioncheckmesh))
  (bind (_outhit _returnvalue) (Collision|BoxTraceByChannel _origin _origin (* _boxextent 0.8) "0, 0, 0" "TraceTypeQuery4" false (Variables|Default|GetBuildArray) "None" true "(R=1.000000,G=0.000000,B=0.000000,A=1.000000)" "(R=0.000000,G=1.000000,B=0.000000,A=1.000000)" 0.2))
  (if _returnvalue
    (bind _builditem (Class|BuildBPI|GetBuildItem(Message) (.HitActor (Collision|BreakHitResult _outhit))))
    (Utilities|IsValid _builditem
      (:Is%20Valid
        (if (Class|PrimitiveComponent|IsOverlappingComponent (Variables|/Game/DATA/Blueprints/Actors/BuildItems/BP_MasterBuild.BP_MasterBuild_C|GetCollisionCheckMesh _builditem) (Variables|/Game/DATA/Blueprints/Actors/BuildItems/BP_MasterBuild.BP_MasterBuild_C|GetCollisionCheckMesh Target))
          (return false)
          (else
            (return true))))
      (:Is%20Not%20Valid
        (return false)))
    (else
      (return true))))

(fn CanBuild
  (LocalVariables|SetL_OverlapCount 0)
  (for _array_element (Variables|Default|GetBuildArray)
    (bind _returnvalue (CallFunction|ChechforOverlap _array_element))
    (if _returnvalue
      (Default|GiveBuildColor _array_element true)
      (else
        (Default|GiveBuildColor _array_element false)
        (Math|Integer|IncrementInt (LocalVariables|GetL_OverlapCount)))))
  (return (< (LocalVariables|GetL_OverlapCount) 1)))

(fn GetBuildType
  (params (Build%20Actor :type BP%20Master%20Build%20Object%20Reference))
  (for _array_element (Variables|/Game/DATA/Blueprints/Components/BuildComponent.BuildComponent_C|GetBuildables (Variables|/Game/DATA/BP_BuildPawn.BP_BuildPawn_C|GetBuildComponent (Variables|Default|GetPlayer)))
    (if (== (.buildactor _array_element) (Utilities|GetClass Build%20Actor))
      (return (.buildtype _array_element)))))

(fn Place
  (for _array_element (Variables|Default|GetBuildArray)
    (if (or (Utilities|Enum|Equal(Enum) (CallFunction|GetBuildType _array_element) "NewEnumerator8") (Utilities|Enum|Equal(Enum) (CallFunction|GetBuildType _array_element) "NewEnumerator1"))
      (Default|AddFoundationExtension _array_element))
    (Default|SetGrey _array_element)
    (Transformation|DetachFromActor _array_element "KeepWorld" "KeepWorld" "KeepWorld"))
  (Utilities|Array|Clear (Variables|Default|GetBuildArray)))

(fn RemoveUI
  (bind _savemenu (Variables|Default|GetSaveMenu)
    (:then
      (Widget|RemovefromParent _savemenu))
    (:else
      _))
  (bind _blueprintmenu (Variables|Default|GetBlueprintMenu)
    (:then
      (Widget|RemovefromParent _blueprintmenu))
    (:else)))