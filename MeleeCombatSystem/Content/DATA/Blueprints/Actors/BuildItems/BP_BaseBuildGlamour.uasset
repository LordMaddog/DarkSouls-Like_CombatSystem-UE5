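; Base buildable glamour station with double doors that open to give the player a glamour inventory UI.
; Interact events toggle a timeline that swings both doors and hides the prompt while moving; Deactivate reverses it.
; When the timeline finishes with the player in the sphere, it restores the prompt and shows or collapses the glamour UI.
; The UI comes from the player's main inventory widget, is filled from the InventoryComponent, and toggles the mouse cursor.
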(event Custom|Glamour
  (if (Variables|Default|GetInteractON)
    (CallFunction|OpenGlamourUI)
    (else
      (CallFunction|CloseGlamourUI))))

(event EventBeginPlay
  (|CallParentFunction) ; This node is disabled and will not be called.\nDrag off pins to build functionality.
)

(event EventDeactivate
  (Variables|Default|SetInteractON false)
  (Variables|/Script/UMG.TextBlock|SetText (Variables|Default|GetText) "Oppen Doors")
  (bind _oppenclose (Timeline|Timeline ReverseFromEnd)
    (:Update
      (Variables|Default|SetInteractActive true)
      (Transformation|SetRelativeRotation (Variables|Default|GetDoorRight) (Math|Rotator|Lerp(Rotator) "0, 0, 0" "0.000000,110.000000,0.000000" _oppenclose) false false)
      (Transformation|SetRelativeRotation (Variables|Default|GetDoorLeft) (Math|Rotator|Lerp(Rotator) "0, 0, 0" "0.000000,-110.000000,0.000000" _oppenclose) false false)
      (Rendering|SetVisibility (Variables|Default|GetInteractText) false false))
    (:Finished
      (Variables|Default|SetInteractActive false)
      (if (Variables|Default|GetInSphere)
        (Rendering|SetVisibility (Variables|Default|GetInteractText) true false)
        (CallFunction|Glamour)))))

(event EventInteractActivate
  (if (and (Variables|Default|GetIsBuildDone) (not (Variables|Default|GetInteractActive)))
    (Variables|Default|SetInteractON true)
    (Variables|/Script/UMG.TextBlock|SetText (Variables|Default|GetText) "Close Doors")
    (bind _oppenclose (Timeline|Timeline PlayFromStart)
      (:Update
        (Variables|Default|SetInteractActive true)
        (Transformation|SetRelativeRotation (Variables|Default|GetDoorRight) (Math|Rotator|Lerp(Rotator) "0, 0, 0" "0.000000,110.000000,0.000000" _oppenclose) false false)
        (Transformation|SetRelativeRotation (Variables|Default|GetDoorLeft) (Math|Rotator|Lerp(Rotator) "0, 0, 0" "0.000000,-110.000000,0.000000" _oppenclose) false false)
        (Rendering|SetVisibility (Variables|Default|GetInteractText) false false))
      (:Finished
        (Variables|Default|SetInteractActive false)
        (if (Variables|Default|GetInSphere)
          (Rendering|SetVisibility (Variables|Default|GetInteractText) true false)
          (CallFunction|Glamour))))))

(event EventInteractStart
  (if (not (Variables|Default|GetInteractActive))
    (Variables|Default|SetInteractActive true)
    (if (not (Variables|Default|GetInteractON))
      (Variables|Default|SetInteractON true)
      (Variables|/Script/UMG.TextBlock|SetText (Variables|Default|GetText) "Close Doors")
      (bind _oppenclose (Timeline|Timeline PlayFromStart)
        (:Update
          (Variables|Default|SetInteractActive true)
          (Transformation|SetRelativeRotation (Variables|Default|GetDoorRight) (Math|Rotator|Lerp(Rotator) "0, 0, 0" "0.000000,110.000000,0.000000" _oppenclose) false false)
          (Transformation|SetRelativeRotation (Variables|Default|GetDoorLeft) (Math|Rotator|Lerp(Rotator) "0, 0, 0" "0.000000,-110.000000,0.000000" _oppenclose) false false)
          (Rendering|SetVisibility (Variables|Default|GetInteractText) false false))
        (:Finished
          (Variables|Default|SetInteractActive false)
          (if (Variables|Default|GetInSphere)
            (Rendering|SetVisibility (Variables|Default|GetInteractText) true false)
            (CallFunction|Glamour))))
      (else
        (Variables|Default|SetInteractON false)
        (Variables|/Script/UMG.TextBlock|SetText (Variables|Default|GetText) "Oppen Doors")
        (Timeline|Timeline ReverseFromEnd)))))

(event Collision|EventActorBeginOverlap
  (params (OtherActor :type Actor%20Object%20Reference)))

(event EventTick
  (params (DeltaSeconds :type Float%20%28single-precision%29)))

(fn ConstructionScript
  (|CallParentFunction))

(fn OpenGlamourUI
  (bind _inventorycomponent (Variables|Default|GetInventoryComponent))
  (Utilities|IsValid (Variables|Default|GetGlamourUI)
    (:Is%20Valid
      _)
    (:Is%20Not%20Valid
      (Variables|Default|SetGlamourUI (Variables|/Game/DATA/UI/Inventory/WBP_MainWidget.WBP_MainWidget_C|GetWBP_GlamourUI (Variables|/Game/DATA/Blueprints/Actors/Inventory/BP_Inventory.BP_Inventory_C|GetMainWidget (Variables|/Game/DATA/BP_PC.BP_PC_C|GetInventory (Variables|Default|GetPlayer)))))))
  (Widget|SetVisibility (Variables|Default|GetGlamourUI) "Visible")
  (Class|CombatBPI|SetMouseCursorActive(Message) (Variables|/Game/DATA/BP_PC.BP_PC_C|GetPlayer%20Controller (Variables|Default|GetPlayer)) true)
  (Default|GenUpdate (Variables|Default|GetGlamourUI) _inventorycomponent (Variables|/Game/DATA/BP_PC.BP_PC_C|GetInventory (Variables|Default|GetPlayer)) (Variables|/Game/DATA/Blueprints/Components/InventoryComponent.InventoryComponent_C|GetName _inventorycomponent)))

(fn CloseGlamourUI
  (Utilities|IsValid (Variables|Default|GetGlamourUI)
    (:Is%20Valid
      _)
    (:Is%20Not%20Valid
      (Variables|Default|SetGlamourUI (Variables|/Game/DATA/UI/Inventory/WBP_MainWidget.WBP_MainWidget_C|GetWBP_GlamourUI (Variables|/Game/DATA/Blueprints/Actors/Inventory/BP_Inventory.BP_Inventory_C|GetMainWidget (Variables|/Game/DATA/BP_PC.BP_PC_C|GetInventory (Variables|Default|GetPlayer)))))))
  (Widget|SetVisibility (Variables|Default|GetGlamourUI) "Collapsed")
  (Class|CombatBPI|SetMouseCursorActive(Message) (Variables|/Game/DATA/BP_PC.BP_PC_C|GetPlayer%20Controller (Variables|Default|GetPlayer)) false)
  (Variables|/Game/DATA/Blueprints/Actors/Inventory/BP_Inventory.BP_Inventory_C|SetActiveInvenComponent (Variables|/Game/DATA/BP_PC.BP_PC_C|GetInventory (Variables|Default|GetPlayer)) 0))