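; Box-shaped elemental hazard area that applies one of five elements (ice, fire, wind, earth, lightning) to characters inside it.
; Persistent areas track overlapping characters and apply elemental damage on a looping timer.
; SelfDelete areas instead hit each non-owner on entry, add a particle burst, then fade out and destroy themselves after LifeTime.
; Construction and BeginPlay activate the element's Niagara effect and sound, scaling both with box size.
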(event OnComponentBeginOverlap(Box)
  (params (OverlappedComponent :type Primitive%20Component%20Object%20Reference) (OtherActor :type Actor%20Object%20Reference) (OtherComp :type Primitive%20Component%20Object%20Reference) (OtherBodyIndex :type Integer) (bFromSweep :type Boolean) (SweepResult :type Hit%20Result%20Structure%20%28by%20ref%29))
  ;[1 1 1] Update Overlap
  (bind _character (Class|CombatBPI|GetCharacterInfo(Message) OtherActor))
  (Utilities|IsValid _character
    (:Is%20Valid
      (if (not (Variables|Default|GetSelfDelete))
        (Utilities|Array|Add (Variables|Default|GetEffectedCharacters) _character)
        (if (== (Utilities|Array|Length (Variables|Default|GetEffectedCharacters)) 1)
          (if (Variables|Default|GetStillActive)
            (Utilities|Time|SetTimerbyFunctionName 0 "ApplyElementalDamage" 0.25 true)))
        (else
          (CallFunction|HitOnce _character))))))

(event OnComponentEndOverlap(Box)
  (params (OverlappedComponent :type Primitive%20Component%20Object%20Reference) (OtherActor :type Actor%20Object%20Reference) (OtherComp :type Primitive%20Component%20Object%20Reference) (OtherBodyIndex :type Integer))
  ;[1 1 1] Update Overlap
  (bind _character (Class|CombatBPI|GetCharacterInfo(Message) OtherActor))
  (Utilities|IsValid _character
    (:Is%20Valid
      (Utilities|Array|RemoveItem (Variables|Default|GetEffectedCharacters) _character)
      (if (== (Utilities|Array|Length (Variables|Default|GetEffectedCharacters)) 0)
        (Utilities|Time|ClearTimerbyFunctionName 0 "ApplyElementalDamage")))))

(event Custom|ApplyElementalDamage
  ;[1 1 1] Apply Elemental Damage
  (for _array_element (Variables|Default|GetEffectedCharacters)
    (Default|ModifyCurrentElement (Variables|/Game/DATA/BP_PC.BP_PC_C|GetStatsComponent _array_element) (Variables|Default|GetElement) (Variables|Default|GetElementalDamage))))

(event Custom|Get%20particleStats
  ;[1 1 1] Test
  (bind (_spawnrate _particlesize) (CallFunction|SetParticleStats))
  (Development|PrintString (Utilities|String|Append "Spawn Rate: " (Utilities|String|ToString(Float) _spawnrate)))
  (Development|PrintString (Utilities|String|Append "Scale: " (Utilities|String|ToString(Float) _particlesize))))

(event EventBeginPlay
  ;[1 1 1] Event Begin play
  (CallFunction|SetParticleStats)
  (if (Variables|Default|GetSelfDelete)
    (Utilities|FlowControl|Delay (Variables|Default|GetLifeTime))
    (Variables|Default|SetStillActive false)
    (Utilities|Time|ClearTimerbyFunctionName 0 "ApplyElementalDamage")
    (Components|Activation|Deactivate (Variables|Default|GetN_Fire_Area))
    (Audio|Components|Audio|FadeOut (Variables|Default|GetAreaSound) 1.0 0.0 "Linear" :!class /Script/Engine.AudioComponent)
    (Utilities|FlowControl|Delay 2.0)
    (Actor|DestroyActor)))

(fn ConstructionScript
  (CallFunction|SetParticleStats))

(fn SelectElementalType
  (switch Utilities|FlowControl|Switch|SwitchonE_MagicType (Variables|Default|GetElement)
    (:NewEnumerator1
      (Components|Activation|Activate (Variables|Default|GetN_IceArea) true)
      (CallFunction|SetSound "/Game/DATA/SoundFX/Wind/SC_ReallyColdWind.SC_ReallyColdWind")
      (Audio|Components|Audio|SetVolumeMultiplier (Variables|Default|GetAreaSound) 0.4 :!class /Script/Engine.AudioComponent))
    (:NewEnumerator2
      (Components|Activation|Activate (Variables|Default|GetN_Fire_Area) true)
      (CallFunction|SetSound "/Game/DATA/SoundFX/Fire/SC_FireLowerVolume.SC_FireLowerVolume"))
    (:NewEnumerator5
      (Components|Activation|Activate (Variables|Default|GetN_Wind_Area) true)
      (CallFunction|SetSound "/Game/DATA/SoundFX/Wind/SC_WindSound.SC_WindSound"))
    (:NewEnumerator4
      (Components|Activation|Activate (Variables|Default|GetN_Earth_Area) true)
      (CallFunction|SetSound "/Game/DATA/SoundFX/Earth/BuildingRumble/SC_RockRumbleLooping.SC_RockRumbleLooping"))
    (:NewEnumerator3
      (Components|Activation|Activate (Variables|Default|GetN_Lightning_Area) true)
      (CallFunction|SetSound "/Game/DATA/SoundFX/Lightning/SC_ChannledLighting.SC_ChannledLighting"))))

(fn SetParticleStats
  (bind _box (Variables|Default|GetBox))
  (bind _box_2 (Variables|Default|GetBox))
  (bind _returnvalue (Transformation|GetWorldScale _box))
  (bind _returnvalue_2 (Transformation|GetWorldScale _box_2))
  (bind _returnvalue_3 (* (.x _returnvalue_2) (.y _returnvalue_2) (.z _returnvalue_2)))
  (bind _returnvalue_4 (* (.x _returnvalue) (.y _returnvalue) (.z _returnvalue)))
  (bind _returnvalue_5 (* _returnvalue_4 0.1))
  (bind _returnvalue_6 (* _returnvalue_3 2.0))
  (bind _returnvalue_7 (Math|Float|Clamp(Float) _returnvalue_5 0.5 2.0))
  (Niagara|SetNiagaraVariable(Vector3) (Variables|Default|GetN_IceArea) "EffectArea" (* (Variables|/Script/Engine.BoxComponent|GetBoxExtent (Variables|Default|GetBox)) 2.0))
  (Niagara|SetNiagaraVariable(Float) (Variables|Default|GetN_IceArea) "SpawnRate" _returnvalue_6)
  (Niagara|SetNiagaraVariable(Float) (Variables|Default|GetN_IceArea) "ParticleSize" _returnvalue_7)
  (if (Variables|Default|GetSelfDelete)
    (Class|NiagaraComponent|SetVariableInt (Variables|Default|GetN_IceArea) "Burst" 20))
  (CallFunction|SelectElementalType)
  (return _returnvalue_6 _returnvalue_7))

(fn HitOnce
  (params (Target :type BP%20PC%20Object%20Reference))
  (if (!= Target (Components|GetOwner))
    (Default|ModifyCurrentElement (Variables|/Game/DATA/BP_PC.BP_PC_C|GetStatsComponent Target) (Variables|Default|GetElement) (Variables|Default|GetElementalDamage))
    (return)))

(fn SetSound
  (params (Selected%20sound :type Sound%20Base%20Object%20Reference))
  (bind _box (Variables|Default|GetBox))
  (bind _returnvalue (Transformation|GetWorldScale _box))
  (bind _returnvalue_2 (* (.x _returnvalue) (.y _returnvalue) (.z _returnvalue)))
  (bind _returnvalue_3 (/ _returnvalue_2 4.0))
  (Audio|Components|Audio|SetSound (Variables|Default|GetAreaSound) Selected%20sound)
  (Audio|Components|Audio|SetVolumeMultiplier (Variables|Default|GetAreaSound) (Math|Float|Clamp(Float) _returnvalue_3 _returnvalue_3 2.0) :!class /Script/Engine.AudioComponent)
  (Components|Activation|Activate (Variables|Default|GetAreaSound) true))