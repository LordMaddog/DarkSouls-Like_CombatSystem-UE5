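; Base actor for armor items, layering armor-specific attachment onto its parent's equip logic.
; AttachActor snaps a valid skeletal mesh to the owning Character's mesh and makes that mesh its leader pose, so the armor follows the body's animation.
; OnEquipped adopts the desired equip type if it is one of four accepted slots, then attaches the static mesh to the character's socket.
; Unequipping defers entirely to the parent.
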(event EventBeginPlay
  (|CallParentFunction) ; This node is disabled and will not be called.\nDrag off pins to build functionality.
)

(event Collision|EventActorBeginOverlap
  (params (OtherActor :type Actor%20Object%20Reference))
  (|CallParentFunction OtherActor) ; This node is disabled and will not be called.\nDrag off pins to build functionality.
)

(event EventTick
  (params (DeltaSeconds :type Float%20%28single-precision%29))
  (|CallParentFunction DeltaSeconds) ; This node is disabled and will not be called.\nDrag off pins to build functionality.
)

(fn ConstructionScript
  (|CallParentFunction))

(fn AttachActor
  (params (SocketName :type Name :default "None") (LocationRule :type EAttachmentRule%20Enum :default "KeepRelative"))
  (bind _returnvalue (Components|GetOwner))
  (bind _ascharacter (Utilities|Casting|CastToCharacter _returnvalue))
  (bind _mesh (Variables|/Script/Engine.Character|GetMesh _ascharacter))
  (Utilities|IsValid (Variables|/Script/Engine.SkeletalMeshComponent|GetSkeletalMeshAsset (Variables|Default|GetItemSkeletalMesh))
    (:Is%20Valid
      (Transformation|AttachComponentToComponent (Variables|Default|GetItemSkeletalMesh) _mesh SocketName "SnapToTarget" "SnapToTarget" "SnapToTarget" true)
      (Components|SkinnedMesh|SetLeaderPoseComponent (Variables|Default|GetItemSkeletalMesh) _mesh true false))))

(fn OnEquipped
  (bind _attachrule (Variables|Default|GetAttachRule))
  (bind _desiredequiptype (Variables|Default|GetDesiredEquipType))
  (|CallParentFunction)
  (if (not (Math|Boolean|ORBoolean (Utilities|Enum|Equal(Enum) _desiredequiptype "NewEnumerator15") (Utilities|Enum|Equal(Enum) _desiredequiptype "NewEnumerator16") (Utilities|Enum|Equal(Enum) _desiredequiptype "NewEnumerator17") (Utilities|Enum|Equal(Enum) _desiredequiptype "NewEnumerator18")))
    _
    (else
      (Variables|Default|SetEquipType (Variables|Default|GetDesiredEquipType))))
  (Transformation|AttachComponentToComponent (Variables|Default|GetItemStaticMesh) (Variables|/Script/Engine.Character|GetMesh (Variables|Default|GetEquipped%20Character)) (Variables|Default|GetAttachSocket%20Name) _attachrule _attachrule _attachrule true))

(fn OnUnequipped
  (params (GiveBack? :type Boolean) (ForceDrop :type Boolean) (ItemInfoIn :type S%20Item%20Info%20Structure))
  (|CallParentFunction GiveBack? ForceDrop ItemInfoIn))