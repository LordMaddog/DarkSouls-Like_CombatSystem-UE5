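; Conversation requirement that gates a dialogue node on the NPC participant's tag message.
; It looks up the actor for its ParticipantTag in the conversation context and reads the tag message from that actor's ConversationComponet.
; It passes when that message equals ParticipantTag.
; A mismatch, missing actor or missing component fails and hides the option.
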(fn IsRequirementSatisfied
  (params (Context :type Conversation%20Context%20Structure%20%28by%20ref%29))
  (bind _returnvalue (Class|ConversationContextHelpers|GetConversationParticipantActor Context (Variables|Default|GetParticipant%20Tag)))
  (Utilities|IsValid _returnvalue
    (:Is%20Valid
      (Utilities|IsValid (Actor|GetComponentbyClass _returnvalue "/Game/DATA/Blueprints/Components/ConversationComponet.ConversationComponet_C")
        (:Is%20Valid
          (bind _tag (Class|ConversationBPI|GetTag(Message) (Actor|GetComponentbyClass _returnvalue "/Game/DATA/Blueprints/Components/ConversationComponet.ConversationComponet_C")))
          (if (== _tag (Variables|Default|GetParticipant%20Tag))
            (return "Passed")
            (else
              (return "FailedAndHidden"))))
        (:Is%20Not%20Valid
          _)))
    (:Is%20Not%20Valid
      _))
  (return "FailedAndHidden"))