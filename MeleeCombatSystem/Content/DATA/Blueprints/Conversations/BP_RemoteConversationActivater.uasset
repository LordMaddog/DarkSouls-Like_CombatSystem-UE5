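; Trigger box actor that remotely starts a conversation on a referenced actor when the player overlaps it.
; If StageRelighent is set, it sends RemoteActivateMessage only when that actor's conversation stage matches Stage.
; ToCastOrNotToCast identifies the player through character info and caches it.
; Once cached, its check compares Player to itself, so any later overlapping actor also passes.
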(event OnComponentBeginOverlap(Box)
  (params (OverlappedComponent :type Primitive%20Component%20Object%20Reference) (OtherActor :type Actor%20Object%20Reference) (OtherComp :type Primitive%20Component%20Object%20Reference) (OtherBodyIndex :type Integer) (bFromSweep :type Boolean) (SweepResult :type Hit%20Result%20Structure%20%28by%20ref%29))
  (bind _isplayer (CallFunction|ToCastorNottoCast OtherActor))
  (if _isplayer
    (if (Variables|Default|GetStageRelighent)
      (bind _stage (Class|ConversationBPI|GetStage(Message) (Variables|/Game/DATA/Blueprints/Actors/World/BP_ConversationNPCBase.BP_ConversationNPCBase_C|GetConversationComponet (Variables|Default|GetActorRef))))
      (if (== _stage (Variables|Default|GetStage))
        (Class|ConversationBPI|RemoteActivate(Message) (Variables|Default|GetActorRef) (Variables|Default|GetPlayer) :!label _label))
      (else
        (goto _label)))))

(fn ConstructionScript)

(fn ToCastorNottoCast
  (params (InActor :type Actor%20Object%20Reference))
  (bind _player (Variables|Default|GetPlayer)
    (:then
      (if (== (Variables|Default|GetPlayer) _player)
        _
        (else
          (return false))))
    (:else
      (bind _character (Class|CombatBPI|GetCharacterInfo(Message) InActor))
      (Utilities|IsValid _character
        (:Is%20Valid
          (if (Variables|/Game/DATA/Blueprints/Components/CombatComponent.CombatComponent_C|GetIsPlayer (Variables|/Game/DATA/BP_PC.BP_PC_C|GetCombatComponent _character))
            (Variables|Default|SetPlayer _character)
            (else
              (return false))))
        (:Is%20Not%20Valid
          (return false)))))
  (return true))