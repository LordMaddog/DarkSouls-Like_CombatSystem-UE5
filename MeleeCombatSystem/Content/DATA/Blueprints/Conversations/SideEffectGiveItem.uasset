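; Conversation side effect that gives the player an item of a configured class with rarity drawn from a configured range.
; On the client, it finds the tagged participant's conversation component and passes the class and rarity bounds to its give-item message.
; A separate helper, not called in this graph, spawns a temporary item to generate rarity, flags it for self-deletion and adds its info to the player's inventory.
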(fn ClientCauseSideEffect
  (params (Context :type Conversation%20Context%20Structure%20%28by%20ref%29))
  (bind _rarityrange (Variables|Default|GetRarityRange))
  (bind _returnvalue (Class|ConversationContextHelpers|GetConversationParticipantActor Context (Variables|Default|GetParticipant%20Tag)))
  (Utilities|IsValid _returnvalue
    (:Is%20Valid
      (Utilities|IsValid (Actor|GetComponentbyClass _returnvalue "/Game/DATA/Blueprints/Components/ConversationComponet.ConversationComponet_C")
        (:Is%20Valid
          (Class|ConversationBPI|GiveItemtoPlayer(Message) (Actor|GetComponentbyClass _returnvalue "/Game/DATA/Blueprints/Components/ConversationComponet.ConversationComponet_C") (Variables|Default|GetClass) (Math|Float|Truncate (.basevalue _rarityrange)) (Math|Float|Truncate (.maxvalue _rarityrange)))
          (return))))))

(fn SpawnItemandGenerateRarity
  (params (Player :type BP%20PC%20Object%20Reference))
  (bind _rarityrange (Variables|Default|GetRarityRange))
  (bind _class (Variables|Default|GetClass))
  (bind _inventory (Variables|/Game/DATA/BP_PC.BP_PC_C|GetInventory Player))
  (LocalVariables|SetRarity (Utilities|Enum|ByteToEnumE_Rarity (Math|Conversions|ToByte(Integer) (Math|Random|RandomIntegerinRange (Math|Float|Truncate (.basevalue _rarityrange)) (Math|Float|Truncate (.maxvalue _rarityrange))))))
  (bind _returnvalue (Game|SpawnActorfromClass _class (Math|Transform|MakeTransform "0, 0, 0" "0, 0, 0" "1.000000,1.000000,1.000000") "Undefined" "MultiplyWithRoot" 0 (Utilities|GetClassDefaults _class) "NewEnumerator0" 1 "NewEnumerator7" "NewEnumerator0" 0 0 0 (LocalVariables|GetRarity) true 0))
  (Variables|/Game/DATA/Blueprints/Actors/BP_MasterItem.BP_MasterItem_C|SetGenerateRarity _returnvalue false)
  (Default|GenerateRarity _returnvalue 0.0)
  (Default|AutoDeleteSelf _returnvalue)
  (Default|AddItemAlt _inventory (Variables|/Game/DATA/Blueprints/Actors/BP_MasterItem.BP_MasterItem_C|GetItemInfo _returnvalue) (Variables|Default|GetClass) 1 true (Variables|/Game/DATA/Blueprints/Actors/Inventory/BP_Inventory.BP_Inventory_C|GetSlots _inventory))
  (return))