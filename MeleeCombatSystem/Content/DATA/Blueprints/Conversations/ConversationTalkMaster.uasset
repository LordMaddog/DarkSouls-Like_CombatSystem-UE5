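; A conversation task node that delivers one line of dialogue through a participant's conversation component.
; It finds the actor by ParticipantTag and passes the portrait, name, text, input prompts and display timing to that component's dialogue UI.
; Optional flags advance the component's stage message or pause the conversation and send the line to client choices, otherwise it returns an empty result.
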(fn ExecuteTaskNode
  (params (Context :type Conversation%20Context%20Structure%20%28by%20ref%29))
  (bind _returnvalue (Class|ConversationContextHelpers|GetConversationParticipantActor Context (Variables|Default|GetParticipant%20Tag)))
  (bind _output_get (LocalVariables|SetParticipant _returnvalue))
  (Utilities|IsValid _output_get
    (:Is%20Valid
      (Utilities|IsValid (Actor|GetComponentbyClass (LocalVariables|GetParticipant) "/Game/DATA/Blueprints/Components/ConversationComponet.ConversationComponet_C")
        (:Is%20Valid
          (bind _output_get_2 (LocalVariables|SetConversationComponent (Actor|GetComponentbyClass (LocalVariables|GetParticipant) "/Game/DATA/Blueprints/Components/ConversationComponet.ConversationComponet_C")))
          (Class|ConversationBPI|UpdateDialogueUI(Message) _output_get_2 (Variables|Default|GetPortrait) (Variables|Default|GetName) (Variables|Default|GetDialoge) (Variables|Default|GetKey%20Instruction) (Variables|Default|GetInput%20Action%20One) (Variables|Default|GetInput%20Action%20Two) (Variables|Default|GetFade) (Variables|Default|GetDisplay%20Duration))
          (if (Variables|Default|GetAdvanceStage)
            (Class|ConversationBPI|ModifyStage(Message) (LocalVariables|GetConversationComponent) 1))
          (if (Variables|Default|GetContinueToTalk)
            (bind _returnvalue_2 (Class|ConversationContextHelpers|PauseConversationandSendClientChoices Context (Utilities|Struct|MakeClientConversationMessage (Variables|Default|GetParticipant%20Tag) (Variables|Default|GetName) (Variables|Default|GetDialoge))))
            (return _returnvalue_2)
            (else
              (return ""))))))))