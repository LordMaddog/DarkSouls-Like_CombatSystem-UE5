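; A conversation side effect node that adds client-side animation, camera zoom and voiced dialogue to a conversation.
; ClientCauseSideEffect resolves the participant actor by ParticipantTag and gets its ConversationComponet, validating both.
; It sends that component messages to play a Montage and Sound when set, and to zoom the camera when Duration exceeds a small threshold.
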(fn ClientCauseSideEffect
  (params (Context :type Conversation%20Context%20Structure%20%28by%20ref%29))
  (bind _returnvalue (Class|ConversationContextHelpers|GetConversationParticipantActor Context (Variables|Default|GetParticipant%20Tag)))
  (Utilities|IsValid _returnvalue
    (:Is%20Valid
      (Utilities|IsValid (Actor|GetComponentbyClass _returnvalue "/Game/DATA/Blueprints/Components/ConversationComponet.ConversationComponet_C")
        (:Is%20Valid
          (Utilities|IsValid (Variables|Default|GetMontage)
            (:Is%20Valid
              (Class|ConversationBPI|PlayAnimation(Message) (Actor|GetComponentbyClass _returnvalue "/Game/DATA/Blueprints/Components/ConversationComponet.ConversationComponet_C") (Variables|Default|GetMontage)))
            (:Is%20Not%20Valid
              _))
          (if (> (Variables|Default|GetDuration) 0.9)
            (Class|ConversationBPI|CameraZoom(Message) (Actor|GetComponentbyClass _returnvalue "/Game/DATA/Blueprints/Components/ConversationComponet.ConversationComponet_C") (Variables|Default|GetDuration)))
          (Utilities|IsValid (Variables|Default|GetSound)
            (:Is%20Valid
              (Class|ConversationBPI|PlayVoicedDialogue(Message) (Actor|GetComponentbyClass _returnvalue "/Game/DATA/Blueprints/Components/ConversationComponet.ConversationComponet_C") (Variables|Default|GetSound)))
            (:Is%20Not%20Valid
              _))
          (return))))))