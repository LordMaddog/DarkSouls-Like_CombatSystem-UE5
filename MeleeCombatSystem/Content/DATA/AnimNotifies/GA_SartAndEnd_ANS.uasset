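; Anim notify state that marks the active window of a GA on the owner's CombatComponent.
; On begin it sends GAActiveMessage with its Hand setting.
; On end it sends GAStopMessage, except when a BP_PC owner's current montage is still the LinkedAnimation, which lets the active state carry on.
; Owners that are not BP_PC always get the stop message.
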(fn ReceivedNotifyBegin
  (params (MeshComp :type Skeletal%20Mesh%20Component%20Object%20Reference) (Animation :type Anim%20Sequence%20Base%20Object%20Reference) (TotalDuration :type Float%20%28single-precision%29) (EventReference :type Anim%20Notify%20Event%20Reference%20Structure%20%28by%20ref%29))
  (Class|CombatBPI|GAActive(Message) (Actor|GetComponentbyClass (Components|GetOwner MeshComp) "/Game/DATA/Blueprints/Components/CombatComponent.CombatComponent_C") (Variables|Default|GetHand))
  (return true))

(fn ReceivedNotifyEnd
  (params (MeshComp :type Skeletal%20Mesh%20Component%20Object%20Reference) (Animation :type Anim%20Sequence%20Base%20Object%20Reference) (EventReference :type Anim%20Notify%20Event%20Reference%20Structure%20%28by%20ref%29))
  (bind _returnvalue (Components|GetOwner MeshComp))
  (bind _asbp_pc (Utilities|Casting|CastToBP_PC _returnvalue)
    (:then
      (if (not (== (Animation|Montage|GetCurrentActiveMontage (Components|SkeletalMesh|GetAnimInstance (Variables|/Script/Engine.Character|GetMesh _asbp_pc))) (Variables|Default|GetLinkedAnimation)))
        _
        (else
          (return false))))
    (:CastFailed
      _))
  (Class|CombatBPI|GAStop(Message) (Actor|GetComponentbyClass _returnvalue "/Game/DATA/Blueprints/Components/CombatComponent.CombatComponent_C"))
  (return true))